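; Checkpoint ring for Speedway courses that the player collects by passing through it.
; Once CourseSpawned is set, a hitbox overlap by the playable character's capsule marks the ring activated, plays a sound and turns it green.
; DeactivateCheckpoint resets it to pink.
; On BeginPlay the ring mesh switches to absolute transform, gets a dynamic material and starts hidden, with its audio muted.
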(event OnComponentBeginOverlap(Ring_Hitbox)
  (params (OverlappedComponent :type Primitive%20Component%20Object%20Reference) (OtherActor :type Actor%20Object%20Reference) (OtherComp :type Primitive%20Component%20Object%20Reference) (OtherBodyIndex :type Integer) (bFromSweep :type Boolean) (SweepResult :type Hit%20Result%20Structure%20%28by%20ref%29))
  (if (Variables|Default|GetCourseSpawned)
    (bind _asbp_base_playable (Utilities|Casting|CastToBP_Base_Playable OtherActor))
    (if (== (Variables|/Script/Engine.Character|GetCapsuleComponent _asbp_base_playable) OtherComp)
      (if (not (Variables|Default|GetisActivated))
        (Audio|PlaySoundatLocation "/Game/SpyroContent/Global_Assets/Global_Level_Items/Gems/Audio/speedway_ring_collected.speedway_ring_collected" (Transformation|GetActorLocation) "0, 0, 0" 1.0 1.0 0.0 0 0 0)
        (Variables|Default|SetisActivated true)
        (Rendering|Material|SetVectorParameterValueonMaterials (Variables|Default|GetStaticMesh) "ColorChange" "0.150000,1.000000,0.000000")))))

(event Custom|DeactivateCheckpoint
  (Variables|Default|SetisActivated false)
  (Rendering|Material|SetVectorParameterValueonMaterials (Variables|Default|GetStaticMesh) "ColorChange" "0.850000,0.000000,1.000000"))

(event EventBeginPlay
  (bind _staticmesh (Variables|Default|GetStaticMesh))
  (Variables|/Script/Engine.SceneComponent|SetbAbsoluteLocation _staticmesh true)
  (Variables|/Script/Engine.SceneComponent|SetbAbsoluteRotation _staticmesh true)
  (Rendering|Material|CreateDynamicMaterialInstance (Variables|Default|GetStaticMesh) 0 "/Game/Speedways/Materials/Speedway_Ring_Pink_Mat.Speedway_Ring_Pink_Mat" "None" :!class /Script/Engine.PrimitiveComponent)
  (Audio|Components|Audio|SetVolumeMultiplier (Variables|Default|GetAudio) 0.0 :!class /Script/Engine.AudioComponent)
  (Rendering|SetVisibility (Variables|Default|GetStaticMesh) false false))

(fn ConstructionScript)