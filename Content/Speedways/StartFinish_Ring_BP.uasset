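; Start/finish ring of a speedway time trial that also hides and later reveals the whole course.
; BeginPlay hides course props and shifts stars and fairies away; SpawnSpeedwayCourse restores them once no essences remain, and ForceSpawnSpeedwayCourse bypasses that check after repeated calls.
; Ring overlaps start a Tick-driven lap timer, invalidate laps with missed checkpoint rings and update the record through the Laptime widget.
; Turbo speedways require Spyro's Superfly, otherwise teleporting him to the spawn point.
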(event OnComponentBeginOverlap(Ring_Hitbox)
  (params (OverlappedComponent :type Primitive%20Component%20Object%20Reference) (OtherActor :type Actor%20Object%20Reference) (OtherComp :type Primitive%20Component%20Object%20Reference) (OtherBodyIndex :type Integer) (bFromSweep :type Boolean) (SweepResult :type Hit%20Result%20Structure%20%28by%20ref%29))
  (if (Variables|Default|GetCourseSpawned)
    (bind _asbp_base_playable (Utilities|Casting|CastToBP_Base_Playable OtherActor))
    (if (== (Variables|/Script/Engine.Character|GetCapsuleComponent _asbp_base_playable) OtherComp)
      (if (Variables|Default|GetisTurboSpeedway)
        (bind _asbp_spyro (Utilities|Casting|CastToBP_Spyro _asbp_base_playable))
        (if (or (Variables|/Game/SpyroContent/Global_Assets/Global_Characters/Playable_Characters/Spyro/BP_Spyro.BP_Spyro_C|GetSuperfly _asbp_spyro) (Variables|/Game/SpyroContent/Global_Assets/Global_Characters/Playable_Characters/Spyro/BP_Spyro.BP_Spyro_C|GetCHEAT_Superfly _asbp_spyro))
          (if (Variables|Default|GetfirstLap) :!label _label
            (for _array_element (Variables|Default|GetmyCheckpoints)
              (bind _asspeedway_ring_bp (Utilities|Casting|CastToSpeedway_Ring_BP _array_element))
              (if (Variables|/Game/Speedways/Speedway_Ring_BP.Speedway_Ring_BP_C|GetisActivated _asspeedway_ring_bp)
                _
                (else
                  (Variables|Default|SetoneOfCheckpointsNotActivated true)))
              (Default|DeactivateCheckpoint _asspeedway_ring_bp))
            (if (Variables|Default|GetoneOfCheckpointsNotActivated)
              (Variables|Default|SetoneOfCheckpointsNotActivated false)
              (Default|UpdateLastLaptime (Variables|Default|GetLaptimeUI) -1.0)
              (Variables|Default|SetCurrent%20Laptime 0.0 :!label _label_2)
              (Audio|PlaySoundatLocation "/Game/SpyroContent/Global_Assets/Global_Level_Items/Gems/Audio/speedway_ring_collected.speedway_ring_collected" (Transformation|GetActorLocation) "0, 0, 0" 1.0 1.0 0.0 0 0 0)
              (else
                (Default|UpdateLastLaptime (Variables|Default|GetLaptimeUI) (Variables|Default|GetCurrent%20Laptime))
                (if (Variables|Default|GetRecord%20Set%20For%20first%20time)
                  (Default|UpdateRecordTime (Variables|Default|GetLaptimeUI) (Variables|Default|GetCurrent%20Laptime) true)
                  (Variables|Default|SetRecord%20Set%20For%20first%20time false)
                  (Variables|Default|SetRecord%20Time (Variables|Default|GetCurrent%20Laptime))
                  (goto _label_2)
                  (elif (< (Variables|Default|GetCurrent%20Laptime) (Variables|Default|GetRecord%20Time))
                    (Default|UpdateRecordTime (Variables|Default|GetLaptimeUI) (Variables|Default|GetCurrent%20Laptime) false)
                    (Variables|Default|SetRecord%20Time (Variables|Default|GetCurrent%20Laptime))
                    (Variables|Default|SetCurrent%20Laptime 0.0)
                    (Audio|PlaySound2D "/Game/SpyroContent/Global_Assets/Global_Level_Items/Butterflies/Audio/1UP.1UP" 1.0 1.0 0.0 0 0)
                    (else
                      (goto _label_2))))))
            (else
              (Variables|Default|SetfirstLap true)
              (Audio|PlaySoundatLocation "/Game/Speedways/SFX/speedway_start.speedway_start" (Transformation|GetActorLocation) "0, 0, 0" 1.0 1.0 0.0 0 0 0)
              (Variables|Default|SetTimer%20Running true)
              (bind _returnvalue (UserInterface|CreateWidget "/Game/Speedways/Laptime.Laptime_C"))
              (bind _output_get (Variables|Default|SetLaptimeUI _returnvalue))
              (UserInterface|Viewport|AddtoViewport _output_get 0)
              (for _array_element_2 (Variables|Default|GetmyCheckpoints)
                (bind _asspeedway_ring_bp_2 (Utilities|Casting|CastToSpeedway_Ring_BP _array_element_2))
                (Default|DeactivateCheckpoint _asspeedway_ring_bp_2)
                (if (Variables|Default|GetisTurboSpeedway)
                  (bind _asbp_spyro_2 (Utilities|Casting|CastToBP_Spyro _asbp_base_playable))
                  (Default|SuperflyBooston _asbp_spyro_2)))))
          (else
            (Game|SpawnActorfromClass "/Game/Speedways/Indicators/BP_GetKissed.BP_GetKissed_C" (Transformation|GetWorldTransform (Variables|Default|GetGetKissedMessageTransform)) "Undefined" 0 0)
            (Transformation|SetActorTransform _asbp_spyro (Variables|Default|GetSpawnTransform) false true)))
        (else
          (goto _label))))))

(event Custom|HideSpeedwayUI
  (bind _laptimeui (Variables|Default|GetLaptimeUI))
  ;[0 0 0] Hide/Show UI
  (Utilities|IsValid _laptimeui
    (:Is%20Valid
      (Widget|SetVisibility _laptimeui "Hidden"))))

(event Custom|ShowSpeedwayUI
  (bind _laptimeui (Variables|Default|GetLaptimeUI))
  ;[0 0 0] Hide/Show UI
  (Utilities|IsValid _laptimeui
    (:Is%20Valid
      (Widget|SetVisibility _laptimeui "Visible"))))

(event Custom|SpawnSpeedwayCourse
  (params (Player%20Who%20Wants%20To%20Spawn%20Me :type BP%20Base%20Playable%20Object%20Reference) (Reset%20Boost%20Enabled :type Boolean))
  (bind _speedway_fairy (Variables|Default|GetSpeedway%20Fairy))
  (bind _timetable (Variables|Default|GetTimetable))
  (bind _speedway_fairy_2 (Variables|Default|GetSpeedway%20Fairy%202))
  (bind _greenballs (Variables|Default|GetGreenBalls))
  (bind _recordrelicinfo (Variables|Default|GetRecordRelicInfo))
  (bind _mesh (Variables|/Script/Engine.Character|GetMesh Player%20Who%20Wants%20To%20Spawn%20Me))
  (bind _returnvalue (Transformation|GetWorldTransform _mesh))
  (bind (_location _rotation) (Math|Transform|BreakTransform _returnvalue))
  (bind (_roll _pitch _yaw) (Math|Rotator|BreakRotator _rotation))
  (if (Variables|Default|GetCourseSpawned)
    (Transformation|SetActorTransform Player%20Who%20Wants%20To%20Spawn%20Me (Variables|Default|GetSpawnTransform) false true)
    (if Reset%20Boost%20Enabled
      _
      (else
        (bind _asbp_spyro (Utilities|Casting|CastToBP_Spyro Player%20Who%20Wants%20To%20Spawn%20Me))
        (Variables|/Game/SpyroContent/Global_Assets/Global_Characters/Playable_Characters/Spyro/BP_Spyro.BP_Spyro_C|SetSuperfly_Speedup _asbp_spyro 0.0)))
    (for _array_element (Variables|Default|GetmyCheckpoints)
      (bind _asspeedway_ring_bp (Utilities|Casting|CastToSpeedway_Ring_BP _array_element))
      (Default|DeactivateCheckpoint _asspeedway_ring_bp))
    (else
      (Variables|Default|SetOneOfEssencesNotCollected false)
      (bind _outactors (Actor|GetAllActorsOfClass "/Game/MeatballsAwaken/Collectibles/Essence/Essence_BP.Essence_BP_C"))
      (for _array_element_2 _outactors
        (Utilities|IsValid _array_element_2
          (:Is%20Valid
            (Variables|Default|SetOneOfEssencesNotCollected true))))
      (if (Variables|Default|GetOneOfEssencesNotCollected)
        (Development|PrintString "Finish the level to spawn speedway course!")
        (Game|SpawnActorfromClass "/Game/Speedways/Indicators/BP_FinishTheLevel.BP_FinishTheLevel_C" (Math|Transform|MakeTransform (+ _location "0, 0,125.000000") (Math|Rotator|MakeRotator _roll _pitch (- _yaw 1.8e+02))) "Undefined" 0 0)
        (else
          (Transformation|SetActorTransform Player%20Who%20Wants%20To%20Spawn%20Me (Variables|Default|GetSpawnTransform) false true)
          (Variables|Default|SetCourseSpawned true)
          (bind _returnvalue_2 (Actor|GetActorOfClass "/Game/SpyroContent/Global_Assets/Global_Level_Items/BP_KillPlane.BP_KillPlane_C"))
          (Utilities|IsValid _returnvalue_2
            (:Is%20Valid
              (Variables|/Game/SpyroContent/Global_Assets/Global_Level_Items/BP_KillPlane.BP_KillPlane_C|SetTeleportsToASpeedway _returnvalue_2 true))
            (:Is%20Not%20Valid
              _))
          (bind _returnvalue_3 (Actor|GetActorOfClass "/Game/SpyroContent/Global_Assets/Global_Level_Items/Drownable_Water/Drownable_Water_BP.Drownable_Water_BP_C"))
          (Utilities|IsValid _returnvalue_3
            (:Is%20Valid
              (Variables|/Game/SpyroContent/Global_Assets/Global_Level_Items/Drownable_Water/Drownable_Water_BP.Drownable_Water_BP_C|SetTeleport%20to%20a%20speedway _returnvalue_3 true))
            (:Is%20Not%20Valid
              _))
          (Rendering|SetVisibility (Variables|Default|GetFlag) true true)
          (Audio|Components|Audio|SetVolumeMultiplier (Variables|Default|GetAudio) 1.0 :!class /Script/Engine.AudioComponent)
          (Rendering|SetVisibility (Variables|Default|GetStaticMesh) true false)
          (for _array_element_3 (Variables|Default|GetSpeedwayRings)
            (bind _asspeedway_ring_bp_2 (Utilities|Casting|CastToSpeedway_Ring_BP _array_element_3))
            (Variables|/Game/Speedways/Speedway_Ring_BP.Speedway_Ring_BP_C|SetCourseSpawned _asspeedway_ring_bp_2 true)
            (Audio|Components|Audio|SetVolumeMultiplier (Variables|/Game/Speedways/Speedway_Ring_BP.Speedway_Ring_BP_C|GetAudio _asspeedway_ring_bp_2) 1.0 :!class /Script/Engine.AudioComponent)
            (Rendering|SetVisibility (Variables|/Game/Speedways/Speedway_Ring_BP.Speedway_Ring_BP_C|GetStaticMesh _asspeedway_ring_bp_2) true false))
          (bind _asred_balls_bp (Utilities|Casting|CastToRed_Balls_BP (Variables|Default|GetRedBalls)))
          (Rendering|SetVisibility (Variables|/Game/Speedways/Red_Balls_BP.Red_Balls_BP_C|GetDefaultSceneRoot _asred_balls_bp) true true)
          (Utilities|IsValid _greenballs
            (:Is%20Valid
              (bind _asgreen_balls_bp (Utilities|Casting|CastToGreen_Balls_BP _greenballs))
              (Rendering|SetVisibility (Variables|/Game/Speedways/Green_Balls_BP.Green_Balls_BP_C|GetDefaultSceneRoot _asgreen_balls_bp) true true))
            (:Is%20Not%20Valid
              _))
          (for (_array_element_4 _array_index) (Variables|Default|GetTransforms-Stars)
            (Transformation|SetActorTransform (Utilities|Array|Get(acopy) (Variables|Default|GetSpeedwayStars) _array_index) _array_element_4))
          (Utilities|IsValid _speedway_fairy
            (:Is%20Valid
              (Transformation|SetActorTransform _speedway_fairy (Variables|Default|GetTransform-SpeedwayFairy)))
            (:Is%20Not%20Valid
              _))
          (Utilities|IsValid _speedway_fairy_2
            (:Is%20Valid
              (Transformation|SetActorTransform _speedway_fairy_2 (Variables|Default|GetTransform-SpeedwayFairy2)))
            (:Is%20Not%20Valid
              _))
          (Utilities|IsValid _timetable
            (:Is%20Valid
              (bind _asbp_timetable (Utilities|Casting|CastToBP_Timetable _timetable))
              (Rendering|SetVisibility (Variables|/Game/Speedways/BP_Timetable.BP_Timetable_C|GetPlane _asbp_timetable) true false))
            (:Is%20Not%20Valid
              _))
          (Utilities|IsValid _recordrelicinfo
            (:Is%20Valid
              (bind _asbp_record_relic_info (Utilities|Casting|CastToBP_RecordRelicInfo _recordrelicinfo)
                (:then
                  (Rendering|SetVisibility (Variables|/Game/Speedways/BP_RecordRelicInfo.BP_RecordRelicInfo_C|GetPlane _asbp_record_relic_info) true false))
                (:CastFailed
                  _)))
            (:Is%20Not%20Valid
              _))
          (for _array_element_5 (Variables|Default|GetActorsToRemove)
            (Actor|DestroyActor _array_element_5))
          (for _array_element_6 (Variables|Default|GetActorsToSpawn)
            (Rendering|SetActorHiddenInGame _array_element_6 false)))))))

(event Custom|ForceSpawnSpeedwayCourse
  (params (Player%20Who%20Wants%20To%20Spawn%20Me :type BP%20Base%20Playable%20Object%20Reference))
  (bind _speedway_fairy (Variables|Default|GetSpeedway%20Fairy))
  (bind _timetable (Variables|Default|GetTimetable))
  (bind _speedway_fairy_2 (Variables|Default|GetSpeedway%20Fairy%202))
  (bind _greenballs (Variables|Default|GetGreenBalls))
  (bind _recordrelicinfo (Variables|Default|GetRecordRelicInfo))
  (if (== (Variables|Default|GetForceSpawnCount) 2)
    (if (not (Variables|Default|GetCourseSpawned))
      (Variables|Default|SetCourseSpawned true)
      (Transformation|SetActorTransform Player%20Who%20Wants%20To%20Spawn%20Me (Variables|Default|GetSpawnTransform) false true)
      (bind _returnvalue (Actor|GetActorOfClass "/Game/SpyroContent/Global_Assets/Global_Level_Items/BP_KillPlane.BP_KillPlane_C"))
      (Utilities|IsValid _returnvalue
        (:Is%20Valid
          (Variables|/Game/SpyroContent/Global_Assets/Global_Level_Items/BP_KillPlane.BP_KillPlane_C|SetTeleportsToASpeedway _returnvalue true))
        (:Is%20Not%20Valid
          _))
      (bind _returnvalue_2 (Actor|GetActorOfClass "/Game/SpyroContent/Global_Assets/Global_Level_Items/Drownable_Water/Drownable_Water_BP.Drownable_Water_BP_C"))
      (Utilities|IsValid _returnvalue_2
        (:Is%20Valid
          (Variables|/Game/SpyroContent/Global_Assets/Global_Level_Items/Drownable_Water/Drownable_Water_BP.Drownable_Water_BP_C|SetTeleport%20to%20a%20speedway _returnvalue_2 true))
        (:Is%20Not%20Valid
          _))
      (Rendering|SetVisibility (Variables|Default|GetFlag) true true)
      (Audio|Components|Audio|SetVolumeMultiplier (Variables|Default|GetAudio) 1.0 :!class /Script/Engine.AudioComponent)
      (Rendering|SetVisibility (Variables|Default|GetStaticMesh) true false)
      (for _array_element (Variables|Default|GetSpeedwayRings)
        (bind _asspeedway_ring_bp (Utilities|Casting|CastToSpeedway_Ring_BP _array_element))
        (Variables|/Game/Speedways/Speedway_Ring_BP.Speedway_Ring_BP_C|SetCourseSpawned _asspeedway_ring_bp true)
        (Audio|Components|Audio|SetVolumeMultiplier (Variables|/Game/Speedways/Speedway_Ring_BP.Speedway_Ring_BP_C|GetAudio _asspeedway_ring_bp) 1.0 :!class /Script/Engine.AudioComponent)
        (Rendering|SetVisibility (Variables|/Game/Speedways/Speedway_Ring_BP.Speedway_Ring_BP_C|GetStaticMesh _asspeedway_ring_bp) true false))
      (bind _asred_balls_bp (Utilities|Casting|CastToRed_Balls_BP (Variables|Default|GetRedBalls)))
      (Rendering|SetVisibility (Variables|/Game/Speedways/Red_Balls_BP.Red_Balls_BP_C|GetDefaultSceneRoot _asred_balls_bp) true true)
      (Utilities|IsValid _greenballs
        (:Is%20Valid
          (bind _asgreen_balls_bp (Utilities|Casting|CastToGreen_Balls_BP _greenballs))
          (Rendering|SetVisibility (Variables|/Game/Speedways/Green_Balls_BP.Green_Balls_BP_C|GetDefaultSceneRoot _asgreen_balls_bp) true true))
        (:Is%20Not%20Valid
          _))
      (for (_array_element_2 _array_index) (Variables|Default|GetTransforms-Stars)
        (Transformation|SetActorTransform (Utilities|Array|Get(acopy) (Variables|Default|GetSpeedwayStars) _array_index) _array_element_2))
      (Utilities|IsValid _speedway_fairy
        (:Is%20Valid
          (Transformation|SetActorTransform _speedway_fairy (Variables|Default|GetTransform-SpeedwayFairy)))
        (:Is%20Not%20Valid
          _))
      (Utilities|IsValid _speedway_fairy_2
        (:Is%20Valid
          (Transformation|SetActorTransform _speedway_fairy_2 (Variables|Default|GetTransform-SpeedwayFairy2)))
        (:Is%20Not%20Valid
          _))
      (Utilities|IsValid _timetable
        (:Is%20Valid
          (bind _asbp_timetable (Utilities|Casting|CastToBP_Timetable _timetable))
          (Rendering|SetVisibility (Variables|/Game/Speedways/BP_Timetable.BP_Timetable_C|GetPlane _asbp_timetable) true false))
        (:Is%20Not%20Valid
          _))
      (Utilities|IsValid _recordrelicinfo
        (:Is%20Valid
          (bind _asbp_record_relic_info (Utilities|Casting|CastToBP_RecordRelicInfo _recordrelicinfo)
            (:then
              (Rendering|SetVisibility (Variables|/Game/Speedways/BP_RecordRelicInfo.BP_RecordRelicInfo_C|GetPlane _asbp_record_relic_info) true false))
            (:CastFailed
              _)))
        (:Is%20Not%20Valid
          _))
      (for _array_element_3 (Variables|Default|GetActorsToRemove)
        (Actor|DestroyActor _array_element_3))
      (for _array_element_4 (Variables|Default|GetActorsToSpawn)
        (Rendering|SetActorHiddenInGame _array_element_4 false)))
    (else
      (Variables|Default|SetForceSpawnCount (+ (Variables|Default|GetForceSpawnCount) 1)))))

(event EventBeginPlay
  (bind _speedway_fairy (Variables|Default|GetSpeedway%20Fairy))
  (bind _speedway_fairy_2 (Variables|Default|GetSpeedway%20Fairy%202))
  (bind _staticmesh (Variables|Default|GetStaticMesh))
  (Variables|Default|SetSpawnTransform (Transformation|GetWorldTransform (Variables|Default|GetSpawnPoint)))
  (Rendering|SetVisibility (Variables|Default|GetFlag) false true)
  (Variables|/Script/Engine.SceneComponent|SetbAbsoluteLocation _staticmesh true)
  (Variables|/Script/Engine.SceneComponent|SetbAbsoluteRotation _staticmesh true)
  (bind _outactors (Actor|GetAllActorsOfClass "/Game/Speedways/Speedway_Ring_BP.Speedway_Ring_BP_C"))
  (Variables|Default|SetmyCheckpoints _outactors)
  ;[0 0 0 1 11] Without this delay, fairies will respawn Spyro -15000 unreal units below than they should
  (Utilities|FlowControl|Delay 0.1)
  (Audio|Components|Audio|SetVolumeMultiplier (Variables|Default|GetAudio) 0.0 :!class /Script/Engine.AudioComponent)
  (Rendering|SetVisibility (Variables|Default|GetStaticMesh) false false)
  ;[0 0 0] Red and green spheres
  (bind _returnvalue (Actor|GetActorOfClass "/Game/Speedways/Red_Balls_BP.Red_Balls_BP_C"))
  (Variables|Default|SetRedBalls _returnvalue)
  (Rendering|SetVisibility (Variables|/Game/Speedways/Red_Balls_BP.Red_Balls_BP_C|GetDefaultSceneRoot _returnvalue) false true)
  (bind _returnvalue_2 (Actor|GetActorOfClass "/Game/Speedways/Green_Balls_BP.Green_Balls_BP_C"))
  (Utilities|IsValid _returnvalue_2
    (:Is%20Valid
      (Variables|Default|SetGreenBalls _returnvalue_2)
      (Rendering|SetVisibility (Variables|/Game/Speedways/Green_Balls_BP.Green_Balls_BP_C|GetDefaultSceneRoot _returnvalue_2) false true))
    (:Is%20Not%20Valid
      _))
  (bind _outactors_2 (Actor|GetAllActorsOfClass "/Game/Speedways/Speedway_Ring_BP.Speedway_Ring_BP_C"))
  (Variables|Default|SetSpeedwayRings _outactors_2)
  ;[0 0 0] Blue stars
  (bind _outactors_3 (Actor|GetAllActorsOfClass "/Game/qtdergContent/Level_Items/BlueStar_Modified_BP.BlueStar_Modified_BP_C"))
  (Variables|Default|SetSpeedwayStars _outactors_3)
  (for _array_element _outactors_3
    (Utilities|Array|Add (Variables|Default|GetTransforms-Stars) (Transformation|GetActorTransform _array_element))
    (Transformation|SetActorTransform _array_element (Math|Transform|MakeTransform (Math|Vector|MakeVector (.X (Math|Vector|BreakVector (.Location (Math|Transform|BreakTransform (Transformation|GetActorTransform _array_element))))) (.Y (Math|Vector|BreakVector (.Location (Math|Transform|BreakTransform (Transformation|GetActorTransform _array_element))))) (- (.Z (Math|Vector|BreakVector (.Location (Math|Transform|BreakTransform (Transformation|GetActorTransform _array_element))))) 1.5e+04)) (.Rotation (Math|Transform|BreakTransform (Transformation|GetActorTransform _array_element))) (.Scale (Math|Transform|BreakTransform (Transformation|GetActorTransform _array_element))))))
  ;[0 0 0] Fairy
  (Utilities|IsValid _speedway_fairy
    (:Is%20Valid
      (bind _output_get (Variables|Default|SetTransform-SpeedwayFairy (Transformation|GetActorTransform _speedway_fairy)))
      (Transformation|SetActorTransform _speedway_fairy (Math|Transform|MakeTransform (Math|Vector|MakeVector (.X (Math|Vector|BreakVector (.Location (Math|Transform|BreakTransform _output_get)))) (- (.Y (Math|Vector|BreakVector (.Location (Math|Transform|BreakTransform _output_get)))) 2.5e+04) (.Z (Math|Vector|BreakVector (.Location (Math|Transform|BreakTransform _output_get))))) (.Rotation (Math|Transform|BreakTransform _output_get)) (.Scale (Math|Transform|BreakTransform _output_get)))))
    (:Is%20Not%20Valid
      _))
  ;[0 0 0] Fairy 2
  (Utilities|IsValid _speedway_fairy_2
    (:Is%20Valid
      (bind _output_get_2 (Variables|Default|SetTransform-SpeedwayFairy2 (Transformation|GetActorTransform _speedway_fairy_2)))
      (Transformation|SetActorTransform _speedway_fairy_2 (Math|Transform|MakeTransform (Math|Vector|MakeVector (.X (Math|Vector|BreakVector (.Location (Math|Transform|BreakTransform _output_get_2)))) (- (.Y (Math|Vector|BreakVector (.Location (Math|Transform|BreakTransform _output_get_2)))) 2.5e+04) (.Z (Math|Vector|BreakVector (.Location (Math|Transform|BreakTransform _output_get_2))))) (.Rotation (Math|Transform|BreakTransform _output_get_2)) (.Scale (Math|Transform|BreakTransform _output_get_2)))))
    (:Is%20Not%20Valid
      _))
  ;[0 0 0] Timetable
  (bind _returnvalue_3 (Actor|GetActorOfClass "/Game/Speedways/BP_Timetable.BP_Timetable_C"))
  (Utilities|IsValid _returnvalue_3
    (:Is%20Valid
      (Variables|Default|SetTimetable _returnvalue_3)
      (Rendering|SetVisibility (Variables|/Game/Speedways/BP_Timetable.BP_Timetable_C|GetPlane _returnvalue_3) false false)
      ;[0 0 0] Record Relic Info
      (bind _returnvalue_4 (Actor|GetActorOfClass "/Game/Speedways/BP_RecordRelicInfo.BP_RecordRelicInfo_C"))
      (Utilities|IsValid _returnvalue_4
        (:Is%20Valid
          (Variables|Default|SetRecordRelicInfo _returnvalue_4)
          (Rendering|SetVisibility (Variables|/Game/Speedways/BP_RecordRelicInfo.BP_RecordRelicInfo_C|GetPlane _returnvalue_4) false false))
        (:Is%20Not%20Valid
          _))
      (for _array_element_2 (Variables|Default|GetActorsToSpawn)
        (Rendering|SetActorHiddenInGame _array_element_2 true)))))

(event EventTick
  (params (DeltaSeconds :type Float%20%28single-precision%29))
  (if (Variables|Default|GetTimer%20Running)
    (bind _output_get (Variables|Default|SetCurrent%20Laptime (+ DeltaSeconds (Variables|Default|GetCurrent%20Laptime))))
    (Default|UpdateCurrentLaptime (Variables|Default|GetLaptimeUI) _output_get)))

(fn ConstructionScript)