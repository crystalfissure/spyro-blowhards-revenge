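; Red_Balls_BP is a Speedways construction-script actor that places copies of a configurable mesh, presumably red balls, along a spline.
; It divides the spline length by a spacing value, then adds an instance at each interval to a single instanced static mesh component.
; Instances use local-space spline positions with no rotation and unit scale, so they do not turn with the curve.
; The event graph has no active logic.
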(event EventBeginPlay)

(event Collision|EventActorBeginOverlap
  (params (OtherActor :type Actor%20Object%20Reference)))

(event EventTick
  (params (DeltaSeconds :type Float%20%28single-precision%29)))

(fn ConstructionScript
  (Components|StaticMesh|SetStaticMesh (Variables|Default|GetInstancedStaticMesh) (Variables|Default|GetPlaced%20Mesh))
  (bind _output_get (LocalVariables|SetNumberOfInstances (Math|Float|Floor (/ (Spline|GetSplineLength (Variables|Default|GetSpline)) (Variables|Default|GetSpacing)))))
  (for _index (range 0 _output_get)
    (Components|InstancedStaticMesh|AddInstance (Variables|Default|GetInstancedStaticMesh) (Math|Transform|MakeTransform (Spline|GetLocationatDistanceAlongSpline (Variables|Default|GetSpline) (* _index (Variables|Default|GetSpacing)) "Local")))))