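; Snowman_BP is a damageable snowman actor, filed under the game's Fodder content.
; On BeginPlay it calls the parent logic and assigns its Hitbox to the Damageable component as the object's hitbox.
; When Damageable reports damage successfully dealt, it plays the Snowman_yeowch sound at the actor's location.
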(event DamageWasSuccessfullyDealt(Damageable)
  (Audio|PlaySoundatLocation "/Game/MeatballsAwaken/Fodder/Snowman/Snowman_yeowch.Snowman_yeowch" (Transformation|GetActorLocation) "0, 0, 0" 1.0 1.0 0.0 0 0 0))

(event EventBeginPlay
  (|CallParentFunction)
  (Variables|/Game/SpyroContent/Global_Assets/Global_Components/Damageable_Com.Damageable_Com_C|SetObject's%20Hitbox%20Component (Variables|Default|GetDamageable) (Variables|Default|GetHitbox)))

(event EventTick
  (params (DeltaSeconds :type Float%20%28single-precision%29))
  (|CallParentFunction DeltaSeconds) ; This node is disabled and will not be called.\nDrag off pins to build functionality.
)

(fn ConstructionScript
  (|CallParentFunction))