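; Sunny Villa tree prop that reacts to damage through a damageable component using its capsule as the hitbox.
; One damage type burns it once: it sets IsBurned, broadcasts the burn, spawns burning VFX and fades a dynamic material's ColorChange by timeline.
; When the fade finishes, the mesh and materials swap to burned versions.
; Another damage type plays a pitch-rotation timeline on the mesh, gated until it finishes.
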(event CallDealDamage(Damageable_Com)
  (bind _staticmesh (Variables|Default|GetStaticMesh))
  (if (Utilities|Enum|Equal(Enum) (Variables|/Game/SpyroContent/Global_Assets/Global_Components/Damageable_Com.Damageable_Com_C|GetDeal%20Damage%20-%20Damage%20Type (Variables|Default|GetDamageable_Com)) "NewEnumerator1")
    (Utilities|FlowControl|DoOnce false
      (:Completed
        (Variables|Default|Setis%20Burned true)
        (Default|CallIHaveBeenBurned!)
        (Effects|SpawnEmitteratLocation "/Game/OT_Ports/S3/S3_Objects/Home_00_SunriseSpring/01_SunnyVilla/Tree/tree_burning_vfx.tree_burning_vfx" (Transformation|GetWorldLocation (Variables|Default|GetEmitter%20spawn%20location)))
        (bind _newtrack_0 (Timeline|Timeline_0 PlayFromStart)
          (:Update
            (Rendering|Material|SetVectorParameterValue (Variables|Default|GetDyn%20Mat%20Ref) "ColorChange" (Utilities|Struct|MakeLinearColor _newtrack_0 _newtrack_0 _newtrack_0 1.0) :!class /Script/Engine.MaterialInstanceDynamic))
          (:Finished
            (Components|StaticMesh|SetStaticMesh _staticmesh "/Game/OT_Ports/S3/S3_Objects/Home_00_SunriseSpring/01_SunnyVilla/Tree/Sunny_Villa_Tree_Burned.Sunny_Villa_Tree_Burned")
            (Rendering|Material|SetMaterial _staticmesh 1 "/Game/SpyroContent/Global_Assets/Global_Materials/Material_Instances/Untex_Vertex_Color_2Sided.Untex_Vertex_Color_2Sided")
            (Rendering|Material|SetMaterial _staticmesh 0 "/Game/OT_Ports/S3/S3_Objects/Home_00_SunriseSpring/01_SunnyVilla/Tree/Sunny_Villa_Tree_Burned_Mat.Sunny_Villa_Tree_Burned_Mat")))))
    (elif (Utilities|Enum|Equal(Enum) (Variables|/Game/SpyroContent/Global_Assets/Global_Components/Damageable_Com.Damageable_Com_C|GetDeal%20Damage%20-%20Damage%20Type (Variables|Default|GetDamageable_Com)) "NewEnumerator4")
      (Utilities|FlowControl|DoOnce false :!label _label
        (:Completed
          (bind _newtrack_0_2 (Timeline|Timeline_1 PlayFromStart)
            (:Update
              (Transformation|SetRelativeRotation (Variables|Default|GetStaticMesh) (Math|Rotator|MakeRotator 0.0 _newtrack_0_2 0.0) false false))
            (:Finished
              (goto _label Reset))))))))

(event EventBeginPlay
  (Variables|/Game/SpyroContent/Global_Assets/Global_Components/Damageable_Com.Damageable_Com_C|SetObject's%20Hitbox%20Component (Variables|Default|GetDamageable_Com) (Variables|Default|GetCapsule))
  (bind _returnvalue (Rendering|Material|CreateDynamicMaterialInstance (Variables|Default|GetStaticMesh) 1 "/Game/OT_Ports/S3/S3_Objects/Home_00_SunriseSpring/01_SunnyVilla/Tree/Sunny_Villa_Tree_Mat.Sunny_Villa_Tree_Mat" "None" :!class /Script/Engine.PrimitiveComponent))
  (Variables|Default|SetDyn%20Mat%20Ref _returnvalue))

(fn ConstructionScript)