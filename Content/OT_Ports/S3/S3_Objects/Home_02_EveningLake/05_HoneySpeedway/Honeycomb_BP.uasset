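; Honeycomb speedway ring for Honey Speedway that wraps a child gem as a floating collectible.
; On BeginPlay it disables the gem's physics, Sparx pickup and drop shadow, and sizes its collection radius to the ring hitbox.
; Gem events drive the ring: hiding plays the collection sound and hides it, unhiding restores it, destruction removes it.
; Treasure skin changes refresh the gem's floating appearance; a non-gem child self-destructs the ring.
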(event Custom|My%20Gem%20Hidden
  (Rendering|SetActorHiddenInGame true)
  (Audio|PlaySoundatLocation "/Game/SpyroContent/Global_Assets/Global_Level_Items/Gems/Audio/speedway_ring_collected.speedway_ring_collected" (Transformation|GetActorLocation) "0, 0, 0" 1.0 1.0 0.0 0 0 0))

(event Custom|My%20Gem%20Unhidden
  (Rendering|SetActorHiddenInGame false))

(event Custom|On%20Gem%20Destroyed
  (params (DestroyedActor :type Actor%20Object%20Reference))
  (Rendering|SetActorHiddenInGame true)
  (Utilities|FlowControl|Delay 0.2)
  (Actor|DestroyActor))

(event Custom|On%20Treasure%20Skin%20Changed
  (CallFunction|ManageGem'sFloatingAppearance (Variables|Default|GetChildActor) self))

(event EventBeginPlay
  (bind _staticmesh (Variables|Default|GetStaticMesh))
  (Variables|/Script/Engine.SceneComponent|SetbAbsoluteLocation _staticmesh true)
  (Variables|/Script/Engine.SceneComponent|SetbAbsoluteRotation _staticmesh true)
  (bind _asspyro_persistant_data (Utilities|Casting|CastToSpyro_PersistantData (Game|GetGameInstance))
    (:then
      (EventDispatchers|BindEventtoChangeTreasureSkins _asspyro_persistant_data (delegate Custom|On%20Treasure%20Skin%20Changed)))
    (:CastFailed
      _))
  (bind _asgem_base_bp (Utilities|Casting|CastToGem_Base_BP (Variables|/Script/Engine.ChildActorComponent|GetChildActor (Variables|Default|GetChildActor)))
    (:then
      (Variables|/Game/SpyroContent/Global_Assets/Global_Level_Items/Gems/Actors/Gem_Base_BP.Gem_Base_BP_C|SetFloating _asgem_base_bp true)
      (Variables|/Game/SpyroContent/Global_Assets/Global_Level_Items/Gems/Actors/Gem_Base_BP.Gem_Base_BP_C|SetSparx_Cant_Grab_Me _asgem_base_bp true)
      (Physics|SetSimulatePhysics (Variables|/Game/SpyroContent/Global_Assets/Global_Level_Items/Gems/Actors/Gem_Base_BP.Gem_Base_BP_C|GetCollision_Mesh _asgem_base_bp) false)
      (Game|BindEventtoOnDestroyed _asgem_base_bp (delegate Custom|On%20Gem%20Destroyed))
      (EventDispatchers|BindEventtoGemWasUnhidden _asgem_base_bp (delegate Custom|My%20Gem%20Unhidden))
      (EventDispatchers|BindEventtoGemWasHidden _asgem_base_bp (delegate Custom|My%20Gem%20Hidden))
      (Rendering|SetVisibility (Variables|/Game/SpyroContent/Global_Assets/Global_Level_Items/Gems/Actors/Gem_Base_BP.Gem_Base_BP_C|GetDropshadow _asgem_base_bp) false false)
      (Transformation|SetWorldScale3D (Variables|/Game/SpyroContent/Global_Assets/Global_Level_Items/Gems/Actors/Gem_Base_BP.Gem_Base_BP_C|GetCollection_Radius _asgem_base_bp) (Transformation|GetWorldScale (Variables|Default|GetRing_Hitbox)))
      (Utilities|FlowControl|Delay 0.4)
      (CallFunction|ManageGem'sFloatingAppearance (Variables|Default|GetChildActor) self))
    (:CastFailed
      (Development|PrintString "Gem Ring BP: My child actor is not a gem?????" true true "(R=0.000000,G=0.660000,B=1.000000,A=1.000000)" 2e+01)
      (Actor|DestroyActor))))

(fn ConstructionScript)