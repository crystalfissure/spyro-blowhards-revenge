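; Spyro-style dragon egg/candle collectible, collected by player overlap or a specific damage type, or awarded by an NPC.
; Damageable and NPCAwardItem events drive it, including invulnerability while stolen and auto-collection after the thief dies.
; Collection saves to persistent data, flagging duplicate NPC awards, and may capture the player in a skippable look-at camera cutscene.
; Candles play a lit animation, eggs a timeline rise and spin, before particles and destruction.
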(event OnComponentBeginOverlap(CollectionRadius)
  (params (OverlappedComponent :type Primitive%20Component%20Object%20Reference) (OtherActor :type Actor%20Object%20Reference) (OtherComp :type Primitive%20Component%20Object%20Reference) (OtherBodyIndex :type Integer) (bFromSweep :type Boolean) (SweepResult :type Hit%20Result%20Structure%20%28by%20ref%29))
  (if (not (Variables|Default|GetIs%20stolen%20by%20thief))
    (bind _asbp_base_playable (Utilities|Casting|CastToBP_Base_Playable OtherActor))
    (if (== (Variables|/Script/Engine.Character|GetCapsuleComponent _asbp_base_playable) OtherComp)
      (Variables|Default|SetOverlappingPlayer _asbp_base_playable)
      (if (Variables|Default|GetCanBeCollected)
        (Variables|Default|SetOverlappedCollectionRadius true)
        (CallFunction|CollectEgg _asbp_base_playable)))))

(event Custom|Deal%20Damage%20to%20Dragon%20Candle
  (bind _returnvalue (Utilities|Time|GetWorldDeltaSeconds))
  (bind _damageable (Variables|Default|GetDamageable))
  (if (and (Utilities|Enum|Equal(Enum) (Variables|/Game/SpyroContent/Global_Assets/Global_Components/Damageable_Com.Damageable_Com_C|GetDeal%20Damage%20-%20Damage%20Type _damageable) "NewEnumerator1") (not (Variables|/Game/SpyroContent/Global_Assets/Global_Components/Damageable_Com.Damageable_Com_C|GetInvincible _damageable)))
    (Utilities|FlowControl|DoOnce false
      (:Completed
        (Transformation|DetachFromActor "KeepWorld" "KeepWorld" "KeepWorld")
        (Transformation|SetActorRotation (Math|Rotator|MakeRotator 0.0 0.0 (.yaw (Transformation|GetActorRotation))))
        (if (Variables|Default|GetOverlappedCollectionRadius)
          (bind _output_get (Variables|Default|SetPlayer%20Who%20Lit%20Me%20Ref (stale Custom|Collect%20Egg Base%20Playable%20Ref)))
          (Utilities|IsValid _output_get
            (:Is%20Valid
              (EventDispatchers|BindEventtoPlayerDied (stale _output_get_2) (delegate ifplayerdiesgettingcandlefromnpc) :!label _label)
              (if (Variables|Default|GetOverlappedCollectionRadius)
                (if (Utilities|Enum|Equal(Enum) (Variables|/Game/SpyroContent/Global_Assets/Global_Characters/Playable_Characters/BP_Base_Playable.BP_Base_Playable_C|GetPlayer_State _output_get) "NewEnumerator11")
                  (CallFunction|IfPlayerDiesWhileCollectingCandlefromNpc :!label _label_2))
                (elif (Utilities|Enum|Equal(Enum) (Variables|/Game/SpyroContent/Global_Assets/Global_Characters/Playable_Characters/BP_Base_Playable.BP_Base_Playable_C|GetPlayer_State (stale _output_get_2)) "NewEnumerator11")
                  (goto _label_2)
                  (else
                    _))))
            (:Is%20Not%20Valid
              _))
          (else
            (bind _asbp_base_playable (Utilities|Casting|CastToBP_Base_Playable (Variables|/Game/SpyroContent/Global_Assets/Global_Components/Damageable_Com.Damageable_Com_C|GetDeal%20Damage%20-%20Person%20Who%20Dealt%20the%20Damage (Variables|Default|GetDamageable)))
              (:then
                (bind _output_get_2 (Variables|Default|SetPlayer%20Who%20Lit%20Me%20Ref _asbp_base_playable))
                (Utilities|IsValid _output_get_2
                  (:Is%20Valid
                    (goto _label))
                  (:Is%20Not%20Valid
                    _)))
              (:CastFailed
                _))))
        (|CapturePlayer
          (:then_1
            (Variables|Default|SetCandle%20Floating%20Up true)
            (Components|Animation|PlayAnimation (Variables|Default|GetSkeletalMesh) "/Game/SpyroContent/CiC_Assets/CiC_Level_Items/Dragon_Candle/Animations/dragon_candle_Anim_Armature_Lit.dragon_candle_Anim_Armature_Lit" false)
            (Collision|SetCollisionEnabled (Variables|Default|GetCapsule%20Component) "NoCollision")
            (if (not (Variables|Default|GetisEgg))
              (Utilities|FlowControl|Delay 2.0)
              (Components|Activation|Activate (Variables|Default|GetParticleSystem) false :!label _label_3)
              (Utilities|FlowControl|Delay 0.1)
              (Rendering|SetVisibility (Variables|Default|GetSkeletalMesh) false false)
              (Utilities|FlowControl|Delay 1.9)
              (Actor|DestroyActor)
              (else
                ;[0 0 0] Dragon egg
                (bind (_direction _velocity _rotation_speed) (Timeline|Timeline_1 PlayFromStart)
                  (:Update
                    (Transformation|SetWorldLocationAndRotation (Variables|Default|GetEggMesh) (+ (Math|Vector|MakeVector 0.0 0.0 (select (Variables|Default|GetI%20Am%20An%20NPC%20Award) (* (* _velocity _returnvalue) 62.5) (* (* _velocity _returnvalue) 125.0))) (Transformation|GetWorldLocation (Variables|Default|GetEggMesh))) (Math|Rotator|MakeRotator 0.0 0.0 (+ (* (* _rotation_speed _returnvalue) 125.0) (.Yaw (Math|Rotator|BreakRotator (Transformation|GetWorldRotation (Variables|Default|GetEggMesh)))))) false false))
                  (:Finished
                    (goto _label_3)))))))))))

(event Custom|NPC%20Reward%20Process
  (Variables|Default|SetI%20Am%20An%20NPC%20Award true)
  (bind _player_who_was_awarded_me (Variables|/Game/SpyroContent/Global_Assets/Global_Components/NPC_Award_Item.NPC_Award_Item_C|GetPlayer%20Who%20Was%20Awarded%20Me (Variables|Default|GetNPC_Award_Item))
    (:then
      (CallFunction|CandleGrows)
      (Utilities|FlowControl|Delay 0.5)
      (Default|DealDamage (Variables|Default|GetDamageable) "NewEnumerator1" "0, 0, 0" false _player_who_was_awarded_me false))
    (:else)))

(event Custom|Candle%20Grows
  (bind _newtrack_0 (Timeline|Timeline_0 PlayFromStart)
    (:Update
      (Transformation|SetRelativeScale3D (Variables|Default|GetCapsule%20Component) (Math|Vector|MakeVector _newtrack_0 _newtrack_0 _newtrack_0)))))

(event Custom|Stolen%20By%20Thief
  (Variables|/Game/SpyroContent/Global_Assets/Global_Components/Damageable_Com.Damageable_Com_C|SetInvincible (Variables|Default|GetDamageable) true)
  (Collision|SetCollisionEnabled (Variables|Default|GetCapsule%20Component) "NoCollision")
  (Variables|Default|SetIs%20stolen%20by%20thief true))

(event Custom|Light%20Myself%20After%20Thief%20Dies
  (bind _player_who_was_awarded_me (Variables|/Game/SpyroContent/Global_Assets/Global_Components/NPC_Award_Item.NPC_Award_Item_C|GetPlayer%20Who%20Was%20Awarded%20Me (Variables|Default|GetNPC_Award_Item))
    (:then
      (if (Utilities|ShouldWeCaptureThisPlayer? _player_who_was_awarded_me 2.0)
        (CallFunction|DisableThisPlayer'sInputs _player_who_was_awarded_me)
        (Variables|Default|SetForce%20Candle%20Cutscene true)))
    (:else
      _))
  (Utilities|FlowControl|Delay 2.0)
  (Transformation|DetachFromActor "KeepWorld" "KeepWorld" "KeepWorld")
  (Variables|/Game/SpyroContent/Global_Assets/Global_Components/Damageable_Com.Damageable_Com_C|SetInvincible (Variables|Default|GetDamageable) false)
  (bind _player_who_was_awarded_me_2 (Variables|/Game/SpyroContent/Global_Assets/Global_Components/NPC_Award_Item.NPC_Award_Item_C|GetPlayer%20Who%20Was%20Awarded%20Me (Variables|Default|GetNPC_Award_Item))
    (:then
      (Transformation|SetWorldLocationAndRotation (Variables|Default|GetCamera) (Transformation|GetWorldLocation (Variables|/Game/SpyroContent/Global_Assets/Global_Characters/Playable_Characters/BP_Base_Playable.BP_Base_Playable_C|GetFollowCamera _player_who_was_awarded_me_2)) (Math|Rotator|MakeRotator 0.0 (.pitch (Math|Rotator|FindLookatRotation (Transformation|GetWorldLocation (Variables|/Game/SpyroContent/Global_Assets/Global_Characters/Playable_Characters/BP_Base_Playable.BP_Base_Playable_C|GetFollowCamera _player_who_was_awarded_me_2)) (Transformation|GetWorldLocation (Variables|Default|GetSkeletalMesh)))) (.yaw (Math|Rotator|FindLookatRotation (Transformation|GetWorldLocation (Variables|/Game/SpyroContent/Global_Assets/Global_Characters/Playable_Characters/BP_Base_Playable.BP_Base_Playable_C|GetFollowCamera _player_who_was_awarded_me_2)) (Transformation|GetWorldLocation (Variables|Default|GetSkeletalMesh))))) false false)
      (Default|DealDamage (Variables|Default|GetDamageable) "NewEnumerator1" "0, 0, 0" false _player_who_was_awarded_me_2 false))
    (:else
      (Default|DealDamage (Variables|Default|GetDamageable) "NewEnumerator1" "0, 0, 0" false 0 false))))

(event Custom|Collect%20Egg
  (params (Base%20Playable%20Ref :type BP%20Base%20Playable%20Object%20Reference))
  (bind _returnvalue (Utilities|Time|GetWorldDeltaSeconds))
  (Utilities|FlowControl|DoOnce false
    (:Completed
      (Transformation|DetachFromActor "KeepWorld" "KeepWorld" "KeepWorld")
      (Transformation|SetActorRotation (Math|Rotator|MakeRotator 0.0 0.0 (.yaw (Transformation|GetActorRotation))))
      (if (Variables|Default|GetOverlappedCollectionRadius)
        (bind _output_get (Variables|Default|SetPlayer%20Who%20Lit%20Me%20Ref Base%20Playable%20Ref))
        (Utilities|IsValid _output_get
          (:Is%20Valid
            (EventDispatchers|BindEventtoPlayerDied (stale _output_get_2) (delegate ifplayerdiesgettingcandlefromnpc) :!label _label)
            (if (Variables|Default|GetOverlappedCollectionRadius)
              (if (Utilities|Enum|Equal(Enum) (Variables|/Game/SpyroContent/Global_Assets/Global_Characters/Playable_Characters/BP_Base_Playable.BP_Base_Playable_C|GetPlayer_State _output_get) "NewEnumerator11")
                (CallFunction|IfPlayerDiesWhileCollectingCandlefromNpc :!label _label_2))
              (elif (Utilities|Enum|Equal(Enum) (Variables|/Game/SpyroContent/Global_Assets/Global_Characters/Playable_Characters/BP_Base_Playable.BP_Base_Playable_C|GetPlayer_State (stale _output_get_2)) "NewEnumerator11")
                (goto _label_2)
                (else
                  _))))
          (:Is%20Not%20Valid
            _))
        (else
          (bind _asbp_base_playable (Utilities|Casting|CastToBP_Base_Playable (Variables|/Game/SpyroContent/Global_Assets/Global_Components/Damageable_Com.Damageable_Com_C|GetDeal%20Damage%20-%20Person%20Who%20Dealt%20the%20Damage (Variables|Default|GetDamageable)))
            (:then
              (bind _output_get_2 (Variables|Default|SetPlayer%20Who%20Lit%20Me%20Ref _asbp_base_playable))
              (Utilities|IsValid _output_get_2
                (:Is%20Valid
                  (goto _label))
                (:Is%20Not%20Valid
                  _)))
            (:CastFailed
              _))))
      (|CapturePlayer
        (:then_1
          (Variables|Default|SetCandle%20Floating%20Up true)
          (Components|Animation|PlayAnimation (Variables|Default|GetSkeletalMesh) "/Game/SpyroContent/CiC_Assets/CiC_Level_Items/Dragon_Candle/Animations/dragon_candle_Anim_Armature_Lit.dragon_candle_Anim_Armature_Lit" false)
          (Collision|SetCollisionEnabled (Variables|Default|GetCapsule%20Component) "NoCollision")
          (if (not (Variables|Default|GetisEgg))
            (Utilities|FlowControl|Delay 2.0)
            (Components|Activation|Activate (Variables|Default|GetParticleSystem) false :!label _label_3)
            (Utilities|FlowControl|Delay 0.1)
            (Rendering|SetVisibility (Variables|Default|GetSkeletalMesh) false false)
            (Utilities|FlowControl|Delay 1.9)
            (Actor|DestroyActor)
            (else
              ;[0 0 0] Dragon egg
              (bind (_direction _velocity _rotation_speed) (Timeline|Timeline_1 PlayFromStart)
                (:Update
                  (Transformation|SetWorldLocationAndRotation (Variables|Default|GetEggMesh) (+ (Math|Vector|MakeVector 0.0 0.0 (select (Variables|Default|GetI%20Am%20An%20NPC%20Award) (* (* _velocity _returnvalue) 62.5) (* (* _velocity _returnvalue) 125.0))) (Transformation|GetWorldLocation (Variables|Default|GetEggMesh))) (Math|Rotator|MakeRotator 0.0 0.0 (+ (* (* _rotation_speed _returnvalue) 125.0) (.Yaw (Math|Rotator|BreakRotator (Transformation|GetWorldRotation (Variables|Default|GetEggMesh)))))) false false))
                (:Finished
                  (goto _label_3))))))))))

(event EventBeginPlay
  (bind _damageable (Variables|Default|GetDamageable))
  (bind _npc_award_item (Variables|Default|GetNPC_Award_Item))
  (Variables|/Game/SpyroContent/Global_Assets/Global_Components/Damageable_Com.Damageable_Com_C|SetObject's%20Hitbox%20Component _damageable (Variables|Default|GetHitbox))
  (EventDispatchers|BindEventtoCallDealDamage _damageable (delegate Custom|Deal%20Damage%20to%20Dragon%20Candle))
  (EventDispatchers|BindEventtoNPCAwardSpawned _npc_award_item (delegate Custom|NPC%20Reward%20Process))
  (EventDispatchers|BindEventtoAThiefStoleMe _npc_award_item (delegate Custom|Stolen%20By%20Thief))
  (EventDispatchers|BindEventtoMyThiefDied _npc_award_item (delegate Custom|Light%20Myself%20After%20Thief%20Dies)))

(event EventTick
  (params (DeltaSeconds :type Float%20%28single-precision%29))
  (bind _skeletalmesh (Variables|Default|GetSkeletalMesh))
  (bind _returnvalue (Transformation|GetSocketLocation _skeletalmesh "Bottom"))
  (if (Variables|Default|GetCandle%20Floating%20Up)
    (Transformation|SetWorldRotation (Variables|Default|GetCamera) (Math|Rotator|FindLookatRotation (Transformation|GetWorldLocation (Variables|Default|GetCamera)) (Math|Vector|MakeVector (.x _returnvalue) (.y _returnvalue) (- (.z _returnvalue) 5e+01))) false false)))

(fn ConstructionScript)

(fn AutotalktoNPC?
  (if (Variables|/Game/SpyroContent/Global_Assets/Global_Components/NPC_Award_Item.NPC_Award_Item_C|GetAutotalk%20to%20NPC%20After (Variables|Default|GetNPC_Award_Item))
    (bind _npc_who_awarded_me (Variables|/Game/SpyroContent/Global_Assets/Global_Components/NPC_Award_Item.NPC_Award_Item_C|GetNPC%20Who%20Awarded%20Me (Variables|Default|GetNPC_Award_Item))
      (:then
        (Variables|/Game/SpyroContent/Global_Assets/Global_Characters/NPCs/NPC_Base_BP.NPC_Base_BP_C|SetAutotalks _npc_who_awarded_me true)
        (Default|AutotalkPing _npc_who_awarded_me))
      (:else))))

(fn EnablePlayerInput
  (bind _player_who_lit_me_ref (Variables|Default|GetPlayer%20Who%20Lit%20Me%20Ref)
    (:then
      (bind _spyrocontr_ref (Variables|/Game/SpyroContent/Global_Assets/Global_Characters/Playable_Characters/BP_Base_Playable.BP_Base_Playable_C|GetSpyroContr_Ref _player_who_lit_me_ref)
        (:then
          (Input|EnableInput _player_who_lit_me_ref _spyrocontr_ref)
          (Variables|/Game/SpyroContent/Global_Assets/Global_Characters/Playable_Characters/BP_Base_Playable.BP_Base_Playable_C|SetDid%20we%20disable%20input? _player_who_lit_me_ref false)
          (CallFunction|AutotalktoNPC?)
          (Default|CallPlayerRegainedInput)
          (return))
        (:else)))
    (:else)))

(event Custom|Look%20at%20me
  (Utilities|FlowControl|Delay 0.5)
  (if (not (Variables|Default|GetCutscene%20Was%20Skipped))
    (bind _player_who_lit_me_ref (Variables|Default|GetPlayer%20Who%20Lit%20Me%20Ref)
      (:then
        (Variables|/Game/SpyroContent/Global_Assets/Global_Characters/Playable_Characters/BP_Base_Playable.BP_Base_Playable_C|SetLookAt_Target _player_who_lit_me_ref (Variables|Default|GetSkeletalMesh))
        (Variables|/Game/SpyroContent/Global_Assets/Global_Characters/Playable_Characters/BP_Base_Playable.BP_Base_Playable_C|SetLookAt_Target_SocketName _player_who_lit_me_ref "Bottom"))
      (:else))))

(event Custom|Delayed%20Hide%20Black%20Bars
  (bind _player_who_lit_me_ref (Variables|Default|GetPlayer%20Who%20Lit%20Me%20Ref))
  (Utilities|FlowControl|Delay 2.0)
  (Utilities|FlowControl|DoOnce false
    (:Completed
      (bind _player_who_lit_me_ref_2 (Variables|Default|GetPlayer%20Who%20Lit%20Me%20Ref)
        (:then
          (Default|HideBlackBars (Variables|/Game/SpyroContent/Global_Assets/Global_Characters/Playable_Characters/BP_Base_Playable.BP_Base_Playable_C|GetSpyroContr_Ref _player_who_lit_me_ref_2))
          (Game|Player|SetViewTargetwithBlend (Variables|/Game/SpyroContent/Global_Assets/Global_Characters/Playable_Characters/BP_Base_Playable.BP_Base_Playable_C|GetSpyroContr_Ref _player_who_lit_me_ref) _player_who_lit_me_ref 1.0 "VTBlend_Linear" 0.0 false)
          (Variables|/Game/SpyroContent/Global_Assets/Global_Characters/Playable_Characters/BP_Base_Playable.BP_Base_Playable_C|SetLookAt_Target _player_who_lit_me_ref 0)
          (Utilities|FlowControl|Delay 0.5)
          (CallFunction|Pause/UnpauseMusic self false false)
          (Utilities|FlowControl|DoOnce false
            (:Completed
              (bind _asspyro_player_controller (Utilities|Casting|CastToSpyro_PlayerController (Game|GetPlayerController 0)))
              (if (Utilities|Enum|Equal(Enum) (Variables|Default|GetType%20Of%20Collectable) "NewEnumerator1")
                (Default|ShowPrimaryCollectibleHUD _asspyro_player_controller 3.0))
              (bind _player_who_lit_me_ref_3 (Variables|Default|GetPlayer%20Who%20Lit%20Me%20Ref)
                (:then
                  (Variables|/Game/SpyroContent/Global_Assets/Global_Characters/Playable_Characters/BP_Base_Playable.BP_Base_Playable_C|GetTalking_NPC _player_who_lit_me_ref_3
                    (:then
                      _)
                    (:else
                      (CallFunction|EnablePlayerInput)))
                  (Input|DisableInput (Variables|/Game/SpyroContent/Global_Assets/Global_Characters/Playable_Characters/BP_Base_Playable.BP_Base_Playable_C|GetSpyroContr_Ref _player_who_lit_me_ref_3)))
                (:else
                  _))
              (if (Variables|Default|GetI%20Am%20An%20NPC%20Award)
                (CallFunction|DelayedEnableInput))
              (bind _npc_who_awarded_me (Variables|/Game/SpyroContent/Global_Assets/Global_Components/NPC_Award_Item.NPC_Award_Item_C|GetNPC%20Who%20Awarded%20Me (Variables|Default|GetNPC_Award_Item))
                (:then
                  (Variables|/Game/SpyroContent/Global_Assets/Global_Characters/NPCs/NPC_Base_BP.NPC_Base_BP_C|SetItem%20Award%20is%20Happening _npc_who_awarded_me false))
                (:else
                  _))
              (bind _foundwidgets (Widget|GetAllWidgetsOfClass "/Game/SpyroContent/Global_Assets/Global_UserInterface/Widgets/YouAlreadyHaveThisX.YouAlreadyHaveThisX_C" true))
              (Utilities|IsValid (Utilities|Array|Get(acopy) _foundwidgets)
                (:Is%20Valid
                  (Widget|RemovefromParent (Utilities|Array|Get(acopy) _foundwidgets)))))))
        (:else)))))

(event Custom|Reset%20Players%20Camera
  (Utilities|FlowControl|Delay 1.1)
  (if (not (Variables|Default|GetCutscene%20Was%20Skipped))
    (bind _player_who_lit_me_ref (Variables|Default|GetPlayer%20Who%20Lit%20Me%20Ref)
      (:then
        (Default|InvokedResetCamera _player_who_lit_me_ref))
      (:else))))

(event Custom|Immediate%20Hide%20Black%20Bars
  (bind _player_who_lit_me_ref (Variables|Default|GetPlayer%20Who%20Lit%20Me%20Ref))
  (Utilities|FlowControl|DoOnce false
    (:Completed
      (bind _player_who_lit_me_ref_2 (Variables|Default|GetPlayer%20Who%20Lit%20Me%20Ref)
        (:then
          (Default|HideBlackBars (Variables|/Game/SpyroContent/Global_Assets/Global_Characters/Playable_Characters/BP_Base_Playable.BP_Base_Playable_C|GetSpyroContr_Ref _player_who_lit_me_ref_2))
          (Game|Player|SetViewTargetwithBlend (Variables|/Game/SpyroContent/Global_Assets/Global_Characters/Playable_Characters/BP_Base_Playable.BP_Base_Playable_C|GetSpyroContr_Ref _player_who_lit_me_ref) _player_who_lit_me_ref 1.0 "VTBlend_Linear" 0.0 false)
          (Variables|/Game/SpyroContent/Global_Assets/Global_Characters/Playable_Characters/BP_Base_Playable.BP_Base_Playable_C|SetLookAt_Target _player_who_lit_me_ref 0)
          (Utilities|FlowControl|Delay 0.5)
          (CallFunction|Pause/UnpauseMusic self false false)
          (Utilities|FlowControl|DoOnce false
            (:Completed
              (bind _asspyro_player_controller (Utilities|Casting|CastToSpyro_PlayerController (Game|GetPlayerController 0)))
              (if (Utilities|Enum|Equal(Enum) (Variables|Default|GetType%20Of%20Collectable) "NewEnumerator1")
                (Default|ShowPrimaryCollectibleHUD _asspyro_player_controller 3.0))
              (bind _player_who_lit_me_ref_3 (Variables|Default|GetPlayer%20Who%20Lit%20Me%20Ref)
                (:then
                  (Variables|/Game/SpyroContent/Global_Assets/Global_Characters/Playable_Characters/BP_Base_Playable.BP_Base_Playable_C|GetTalking_NPC _player_who_lit_me_ref_3
                    (:then
                      _)
                    (:else
                      (CallFunction|EnablePlayerInput)))
                  (Input|DisableInput (Variables|/Game/SpyroContent/Global_Assets/Global_Characters/Playable_Characters/BP_Base_Playable.BP_Base_Playable_C|GetSpyroContr_Ref _player_who_lit_me_ref_3)))
                (:else
                  _))
              (if (Variables|Default|GetI%20Am%20An%20NPC%20Award)
                (CallFunction|DelayedEnableInput))
              (bind _npc_who_awarded_me (Variables|/Game/SpyroContent/Global_Assets/Global_Components/NPC_Award_Item.NPC_Award_Item_C|GetNPC%20Who%20Awarded%20Me (Variables|Default|GetNPC_Award_Item))
                (:then
                  (Variables|/Game/SpyroContent/Global_Assets/Global_Characters/NPCs/NPC_Base_BP.NPC_Base_BP_C|SetItem%20Award%20is%20Happening _npc_who_awarded_me false))
                (:else
                  _))
              (bind _foundwidgets (Widget|GetAllWidgetsOfClass "/Game/SpyroContent/Global_Assets/Global_UserInterface/Widgets/YouAlreadyHaveThisX.YouAlreadyHaveThisX_C" true))
              (Utilities|IsValid (Utilities|Array|Get(acopy) _foundwidgets)
                (:Is%20Valid
                  (Widget|RemovefromParent (Utilities|Array|Get(acopy) _foundwidgets)))))))
        (:else)))))

(event Custom|Immediate%20Regain%20Control
  (Utilities|FlowControl|DoOnce false
    (:Completed
      (bind _asspyro_player_controller (Utilities|Casting|CastToSpyro_PlayerController (Game|GetPlayerController 0)))
      (if (Utilities|Enum|Equal(Enum) (Variables|Default|GetType%20Of%20Collectable) "NewEnumerator1")
        (Default|ShowPrimaryCollectibleHUD _asspyro_player_controller 3.0))
      (bind _player_who_lit_me_ref (Variables|Default|GetPlayer%20Who%20Lit%20Me%20Ref)
        (:then
          (Variables|/Game/SpyroContent/Global_Assets/Global_Characters/Playable_Characters/BP_Base_Playable.BP_Base_Playable_C|GetTalking_NPC _player_who_lit_me_ref
            (:then
              _)
            (:else
              (CallFunction|EnablePlayerInput)))
          (Input|DisableInput (Variables|/Game/SpyroContent/Global_Assets/Global_Characters/Playable_Characters/BP_Base_Playable.BP_Base_Playable_C|GetSpyroContr_Ref _player_who_lit_me_ref)))
        (:else
          _))
      (if (Variables|Default|GetI%20Am%20An%20NPC%20Award)
        (CallFunction|DelayedEnableInput))
      (bind _npc_who_awarded_me (Variables|/Game/SpyroContent/Global_Assets/Global_Components/NPC_Award_Item.NPC_Award_Item_C|GetNPC%20Who%20Awarded%20Me (Variables|Default|GetNPC_Award_Item))
        (:then
          (Variables|/Game/SpyroContent/Global_Assets/Global_Characters/NPCs/NPC_Base_BP.NPC_Base_BP_C|SetItem%20Award%20is%20Happening _npc_who_awarded_me false))
        (:else
          _))
      (bind _foundwidgets (Widget|GetAllWidgetsOfClass "/Game/SpyroContent/Global_Assets/Global_UserInterface/Widgets/YouAlreadyHaveThisX.YouAlreadyHaveThisX_C" true))
      (Utilities|IsValid (Utilities|Array|Get(acopy) _foundwidgets)
        (:Is%20Valid
          (Widget|RemovefromParent (Utilities|Array|Get(acopy) _foundwidgets)))))))

(event Custom|Delayed%20Enable%20Input
  (Utilities|FlowControl|Delay 0.5)
  (bind _player_who_lit_me_ref (Variables|Default|GetPlayer%20Who%20Lit%20Me%20Ref)
    (:then
      (Variables|/Game/SpyroContent/Global_Assets/Global_Characters/Playable_Characters/BP_Base_Playable.BP_Base_Playable_C|GetTalking_NPC _player_who_lit_me_ref
        (:then)
        (:else
          _)))
    (:else
      _))
  (CallFunction|EnablePlayerInput))

(event Input|ActionEvents|InputActionPause
  (params (Key :type Key%20Structure :default "None"))
  (:Pressed
    (Utilities|FlowControl|DoOnce false
      (:Completed
        (Variables|Default|SetCutscene%20Was%20Skipped true)
        (CallFunction|ImmediateHideBlackBars)
        (CallFunction|ImmediateRegainControl)))))

(event Input|ActionEvents|InputActionAim/Talk
  (params (Key :type Key%20Structure :default "None"))
  (:Pressed
    (Utilities|FlowControl|DoOnce false
      (:Completed
        (Variables|Default|SetCutscene%20Was%20Skipped true)
        (CallFunction|ImmediateHideBlackBars)
        (CallFunction|ImmediateRegainControl)))))

(event Input|KeyboardEvents|SpaceBar
  (params (Key :type Key%20Structure :default "None"))
  (:Pressed
    (Utilities|FlowControl|DoOnce false
      (:Completed
        (Variables|Default|SetCutscene%20Was%20Skipped true)
        (CallFunction|ImmediateHideBlackBars)
        (CallFunction|ImmediateRegainControl)))))

(event Input|MouseEvents|LeftMouseButton
  (params (Key :type Key%20Structure :default "None"))
  (:Pressed
    (Utilities|FlowControl|DoOnce false
      (:Completed
        (Variables|Default|SetCutscene%20Was%20Skipped true)
        (CallFunction|ImmediateHideBlackBars)
        (CallFunction|ImmediateRegainControl)))))

(event Custom|if%20player%20dies%20while%20collecting%20candle%20from%20npc
  (CallFunction|EnablePlayerInput)
  (CallFunction|DelayedEnableInput))