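; Level quest actor that rewards the player for burning Sunny Villa trees, and destroys itself on BeginPlay if its level bool is already set.
; It binds to each tree's burned event and, after a short delay, recounts burned trees against a target total.
; On completion it saves the level bool and spawns the award item above the player.
; Awards without an NPC_Award_Item component are treated as Skill Point butterflies with an on-screen widget.
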(event Custom|Tree%20Has%20Been%20Burned
  (Utilities|FlowControl|Delay 0.2)
  (bind _total_destroyed (CallFunction|CountTrees))
  (if (== _total_destroyed (Variables|Default|GetTotal%20number%20of%20trees))
    (Utilities|FlowControl|DoOnce false
      (:Completed
        (CallFunction|OnQuestCompletion)))))

(event Custom|On%20Begin%20Play%20If%20Quest%20NOT%20Completed
  (for _array_element (Variables|Default|GetTrees)
    (EventDispatchers|BindEventtoIHaveBeenBurned! _array_element (delegate Custom|Tree%20Has%20Been%20Burned))))

(event Custom|On%20Begin%20Play%20If%20Quest%20IS%20Already%20Completed
  (Actor|DestroyActor))

(event Custom|On%20Quest%20Completion
  (CallFunction|SetLevelBool (Variables|Default|GetCurrent%20Level%20Name) (Variables|Default|GetLevel%20Bool%20ID) self (Class|KismetSystemLibrary|MakeLiteralBool true))
  (bind _returnvalue (Actor|GetActorOfClass "/Game/SpyroContent/Global_Assets/Global_Characters/Playable_Characters/BP_Base_Playable.BP_Base_Playable_C"))
  (bind _returnvalue_2 (Game|SpawnActorfromClass (Variables|Default|GetAward%20Item) (Math|Transform|MakeTransform (+ (Transformation|GetActorLocation _returnvalue) "0, 0,100.000000") "0, 0, 0" "1,1,1") "Undefined" 0 0))
  (Utilities|IsValid (Actor|GetComponentbyClass _returnvalue_2 "/Game/SpyroContent/Global_Assets/Global_Components/NPC_Award_Item.NPC_Award_Item_C")
    (:Is%20Valid
      (Variables|/Game/SpyroContent/Global_Assets/Global_Components/NPC_Award_Item.NPC_Award_Item_C|SetLevel%20Item%20Index (Actor|GetComponentbyClass _returnvalue_2 "/Game/SpyroContent/Global_Assets/Global_Components/NPC_Award_Item.NPC_Award_Item_C") (Variables|Default|GetLevel%20Item%20Index)))
    (:Is%20Not%20Valid
      (bind _asblue_butterfly_bp (Utilities|Casting|CastToBlue_Butterfly_BP _returnvalue_2))
      (Variables|/Game/SpyroContent/Global_Assets/Global_Level_Items/Butterflies/Actors/Blue_Butterfly_BP.Blue_Butterfly_BP_C|SetLevel%20Item%20Index _asblue_butterfly_bp (Variables|Default|GetLevel%20Item%20Index))
      (Variables|/Game/SpyroContent/Global_Assets/Global_Level_Items/Butterflies/Actors/Blue_Butterfly_BP.Blue_Butterfly_BP_C|SetMy_Unique_Name _asblue_butterfly_bp "Skill Point")
      (Variables|/Game/SpyroContent/Global_Assets/Global_Level_Items/Butterflies/Actors/Blue_Butterfly_BP.Blue_Butterfly_BP_C|SetSkill%20Level%20Award _asblue_butterfly_bp 2e+01)
      (bind _asspyro_player_controller (Utilities|Casting|CastToSpyro_PlayerController (Game|GetPlayerController 0)))
      (bind _returnvalue_3 (UserInterface|CreateWidget "/Game/SpyroContent/Global_Assets/Global_UserInterface/Widgets/SkillPoint_Widget.SkillPoint_Widget_C" _asspyro_player_controller))
      (UserInterface|Viewport|AddtoViewport _returnvalue_3 0)
      (Default|HideBottomRightQuestHUD _asspyro_player_controller))))

(event EventBeginPlay
  (bind _outactors (Actor|GetAllActorsOfClass "/Game/OT_Ports/S3/S3_Objects/Home_00_SunriseSpring/01_SunnyVilla/Sunny_Villa_Tree_BP.Sunny_Villa_Tree_BP_C"))
  (Variables|Default|SetTrees _outactors)
  (bind _returnvalue (CallFunction|GetLevelBools (Variables|Default|GetCurrent%20Level%20Name) self))
  (if (Utilities|Array|Get(acopy) _returnvalue (Variables|Default|GetLevel%20Bool%20ID))
    (CallFunction|OnBeginPlayifQuestISAlreadyCompleted)
    (else
      (CallFunction|OnBeginPlayifQuestNOTCompleted))))

(fn ConstructionScript)

(fn CountTrees
  (LocalVariables|SetTotal%20of%20destroyed 0)
  (bind _outactors (Actor|GetAllActorsOfClass "/Game/OT_Ports/S3/S3_Objects/Home_00_SunriseSpring/01_SunnyVilla/Sunny_Villa_Tree_BP.Sunny_Villa_Tree_BP_C"))
  (for _array_element _outactors
    (if (Variables|/Game/OT_Ports/S3/S3_Objects/Home_00_SunriseSpring/01_SunnyVilla/Sunny_Villa_Tree_BP.Sunny_Villa_Tree_BP_C|Getis%20Burned _array_element)
      (Math|Integer|IncrementInt (LocalVariables|GetTotal%20of%20destroyed))))
  (return (LocalVariables|GetTotal%20of%20destroyed)))