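; Quest actor for destroying all Begonias in a level, which ends with an NPC set to award an item.
; On BeginPlay, a saved level bool either removes the NPC and Begonias or binds to each Begonia's damage event.
; Each hit triggers a delayed recount; reaching the total saves completion once, hides the quest HUD and stops Begonias respawning.
; The NPC then gets new dialogue and reward data and teleports to talk to the player.
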(event Custom|Begonia%20Has%20Been%20Destroyed
  (Utilities|FlowControl|Delay 0.2)
  (bind _total_destroyed (CallFunction|CountBegonias))
  (if (== _total_destroyed (Variables|Default|GetTotal%20number%20of%20begonias))
    (Utilities|FlowControl|DoOnce false
      (:Completed
        (CallFunction|OnQuestCompletion)))))

(event Custom|On%20Begin%20Play%20If%20Quest%20NOT%20Completed
  (for _array_element (Variables|Default|GetBegonias)
    (EventDispatchers|BindEventtoContainerSuccessfullyDamaged _array_element (delegate Custom|Begonia%20Has%20Been%20Destroyed))))

(event Custom|On%20Begin%20Play%20If%20Quest%20IS%20Already%20Completed
  (Actor|DestroyActor (Variables|Default|GetNPC%20Ref))
  (for _array_element (Variables|Default|GetBegonias)
    (Actor|DestroyActor _array_element)))

(event Custom|On%20Quest%20Completion
  (bind _npc_ref (Variables|Default|GetNPC%20Ref))
  (CallFunction|SetLevelBool (Variables|Default|GetCurrent%20Level%20Name) (Variables|Default|GetLevel%20Bool%20ID) self (Class|KismetSystemLibrary|MakeLiteralBool true))
  (bind _asspyro_player_controller (Utilities|Casting|CastToSpyro_PlayerController (Game|GetPlayerController 0)))
  (Default|HideBottomRightQuestHUD _asspyro_player_controller)
  (Variables|/Game/SpyroContent/Global_Assets/Global_Characters/NPCs/NPC_Base_BP.NPC_Base_BP_C|SetDialogue_Info _npc_ref (Variables|Default|GetNPC%20dialogue%20after%20destroying%20all%20begonias))
  (Variables|/Game/SpyroContent/Global_Assets/Global_Characters/NPCs/NPC_Base_BP.NPC_Base_BP_C|SetTalk_Again_Dialogue_Info _npc_ref (Variables|Default|GetNPC%20talk%20again%20dialogue%20after%20destroying%20all%20begonias))
  (Variables|/Game/SpyroContent/Global_Assets/Global_Characters/NPCs/NPC_Base_BP.NPC_Base_BP_C|SetLevel%20Item%20Index _npc_ref (Variables|Default|GetLevel%20Item%20Index))
  (Variables|/Game/SpyroContent/Global_Assets/Global_Characters/NPCs/NPC_Base_BP.NPC_Base_BP_C|SetAwards%20an%20Item _npc_ref true)
  (Variables|/Game/SpyroContent/Global_Assets/Global_Characters/NPCs/NPC_Base_BP.NPC_Base_BP_C|SetAward%20Item _npc_ref (Variables|Default|GetAward%20Item))
  (bind _returnvalue (Actor|GetActorOfClass "/Game/SpyroContent/Global_Assets/Global_Characters/Playable_Characters/BP_Base_Playable.BP_Base_Playable_C"))
  (Default|TeleporttoTalktoMe _npc_ref _returnvalue 0.5)
  (for _array_element (Variables|Default|GetBegonias)
    (Variables|/Game/SpyroContent/Global_Assets/Global_Components/Drops_Items.Drops_Items_C|Setnever%20respawn (Variables|/Game/SpyroContent/Global_Assets/Global_Level_Items/Treasure_Containers/Treasure_Container_Base_BP.Treasure_Container_Base_BP_C|GetItem_Drop_Component _array_element) true)))

(event EventBeginPlay
  (bind _outactors (Actor|GetAllActorsOfClass "/Game/SpyroContent/CiC_Assets/CiC_Levels/Home_00_PastChasms/00_PastChasms/Level_Items/Begonias/Begonia_BP.Begonia_BP_C"))
  (Variables|Default|SetBegonias _outactors)
  (bind _returnvalue (CallFunction|GetLevelBools (Variables|Default|GetCurrent%20Level%20Name) self))
  (if (Utilities|Array|Get(acopy) _returnvalue (Variables|Default|GetLevel%20Bool%20ID))
    (CallFunction|OnBeginPlayifQuestISAlreadyCompleted)
    (else
      (CallFunction|OnBeginPlayifQuestNOTCompleted))))

(fn ConstructionScript)

(fn CountBegonias
  (LocalVariables|SetTotal%20of%20destroyed 0)
  (bind _outactors (Actor|GetAllActorsOfClass "/Game/SpyroContent/CiC_Assets/CiC_Levels/Home_00_PastChasms/00_PastChasms/Level_Items/Begonias/Begonia_BP.Begonia_BP_C"))
  (for _array_element _outactors
    (if (Variables|/Game/SpyroContent/Global_Assets/Global_Level_Items/Treasure_Containers/Treasure_Container_Base_BP.Treasure_Container_Base_BP_C|GetContainer_Destroyed _array_element)
      (Math|Integer|IncrementInt (LocalVariables|GetTotal%20of%20destroyed))))
  (return (LocalVariables|GetTotal%20of%20destroyed)))