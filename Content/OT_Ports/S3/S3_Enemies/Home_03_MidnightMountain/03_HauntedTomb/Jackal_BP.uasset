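; Jackal enemy Blueprint for the Haunted Tomb level of Midnight Mountain, extending a parent with walking AI and damageable components.
; At BeginPlay it registers its mesh as the metal-material component and listens for AI state changes.
; Entering the Dying state spawns one burst actor per Shards entry, with randomized height and yaw, to perform the shard burst.
; Weapon hitbox overlaps are forwarded to DamageCheck.
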(event OnComponentBeginOverlap(WeaponHitbox)
  (params (OverlappedComponent :type Primitive%20Component%20Object%20Reference) (OtherActor :type Actor%20Object%20Reference) (OtherComp :type Primitive%20Component%20Object%20Reference) (OtherBodyIndex :type Integer) (bFromSweep :type Boolean) (SweepResult :type Hit%20Result%20Structure%20%28by%20ref%29))
  (CallFunction|DamageCheck OtherActor OtherComp))

(event Custom|Enemy%20State%20Changed
  (bind _returnvalue (Transformation|GetActorTransform))
  (bind (_location _rotation _scale) (Math|Transform|BreakTransform _returnvalue))
  (bind (_x _y _z) (Math|Vector|BreakVector _location))
  (bind (_roll _pitch _yaw) (Math|Rotator|BreakRotator _rotation))
  (switch Utilities|FlowControl|Switch|SwitchonAICharacter_States (Variables|/Game/SpyroContent/Global_Assets/Global_Components/Base_AI_Character.Base_AI_Character_C|GetAICharacter_State (Variables|Default|GetWalking_AI_Character))
    (:NewEnumerator3
      (for _array_element (Variables|Default|GetShards)
        (bind _returnvalue_2 (Game|SpawnActorfromClass "/Game/OT_Ports/Global/Blueprints/Enemy_Burst_BP.Enemy_Burst_BP_C" (Math|Transform|MakeTransform (Math|Vector|MakeVector _x _y (+ _z (Math|Random|RandomFloatinRange -2e+01 0.0))) (Math|Rotator|MakeRotator _roll _pitch (+ _yaw (Math|Random|RandomFloatinRange 0.0 3.6e+02))) _scale) "AlwaysSpawn" 0 0))
        (Default|ShardBurstAction _returnvalue_2 _array_element)))))

(event EventBeginPlay
  (|CallParentFunction)
  (Variables|/Game/SpyroContent/Global_Assets/Global_Components/Damageable_Com.Damageable_Com_C|SetComponent_with_Metal_Material (Variables|Default|GetDamageable) (Variables|Character|GetMesh))
  (EventDispatchers|BindEventtoMyStateChanged (Variables|Default|GetWalking_AI_Character) (delegate Custom|Enemy%20State%20Changed)))

(event Collision|EventActorBeginOverlap
  (params (OtherActor :type Actor%20Object%20Reference)))

(event EventTick
  (params (DeltaSeconds :type Float%20%28single-precision%29))
  (|CallParentFunction DeltaSeconds) ; This node is disabled and will not be called.\nDrag off pins to build functionality.
)

(fn ConstructionScript
  (|CallParentFunction))