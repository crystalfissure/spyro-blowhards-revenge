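; Crystal Flower enemy for Crystal Islands that adds a shatter effect when it dies.
; It listens to its walking AI character's state changes and, on Dying, runs a timeline that shifts the mesh's ColorChange material parameter by varying green and blue.
; When the timeline finishes it plays the death sound, then after a short delay resets the color and spawns a Basket_Burst_BP that throws crystal flower shards.
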(event Custom|Character%20state%20changed
  (bind _mesh (Variables|Character|GetMesh))
  (switch Utilities|FlowControl|Switch|SwitchonAICharacter_States (Variables|/Game/SpyroContent/Global_Assets/Global_Components/Base_AI_Character.Base_AI_Character_C|GetAICharacter_State (Variables|Default|GetWalking_AI_Character))
    (:NewEnumerator3
      (bind _newtrack_0 (Timeline|Timeline_1 PlayFromStart)
        (:Update
          (Rendering|Material|SetVectorParameterValueonMaterials _mesh "ColorChange" (Math|Vector|MakeVector 1.0 _newtrack_0 _newtrack_0)))
        (:Finished
          (Audio|PlaySoundatLocation "/Game/OT_Ports/S3/S3_Enemies/Home_03_MidnightMountain/01_CrystalIslands/Crystal_Flower/Crystal_Flower_Death.Crystal_Flower_Death" (Transformation|GetActorLocation) "0, 0, 0" 1.0 1.0 0.0 "/Game/SpyroContent/Global_Assets/Global_Audio/Attenuation/Spyro_Attenuation_Farther.Spyro_Attenuation_Farther" 0 0)
          (Utilities|FlowControl|Delay 0.2)
          (Rendering|Material|SetVectorParameterValueonMaterials _mesh "ColorChange" "1.000000,1.000000,1.000000")
          (bind _returnvalue (Game|SpawnActorfromClass "/Game/SpyroContent/Global_Assets/Global_Level_Items/Treasure_Containers/Basket/Actors/Basket_Burst_BP.Basket_Burst_BP_C" (Transformation|GetActorTransform) "Undefined" 0 0))
          (Default|ShardBurstAction _returnvalue "/Game/OT_Ports/S3/S3_Enemies/Home_03_MidnightMountain/01_CrystalIslands/Crystal_Flower/Crystal_Flower_Burst.Crystal_Flower_Burst" "/Game/OT_Ports/S3/S3_Enemies/Home_03_MidnightMountain/01_CrystalIslands/Crystal_Flower/Crystal_Flower_Burst.Crystal_Flower_Burst"))))))

(event EventBeginPlay
  (|CallParentFunction)
  (EventDispatchers|BindEventtoMyStateChanged (Variables|Default|GetWalking_AI_Character) (delegate Custom|Character%20state%20changed)))

(event Collision|EventActorBeginOverlap
  (params (OtherActor :type Actor%20Object%20Reference))
  (|CallParentFunction OtherActor) ; This node is disabled and will not be called.\nDrag off pins to build functionality.
)

(event EventTick
  (params (DeltaSeconds :type Float%20%28single-precision%29))
  (|CallParentFunction DeltaSeconds) ; This node is disabled and will not be called.\nDrag off pins to build functionality.
)

(fn ConstructionScript
  (|CallParentFunction))