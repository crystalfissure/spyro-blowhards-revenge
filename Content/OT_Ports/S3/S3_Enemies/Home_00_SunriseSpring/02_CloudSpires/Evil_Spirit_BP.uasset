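; Evil Spirit enemy Blueprint for a Spyro quest, with an idle animation that moves its mesh around a radius and an occasional random laugh.
; On taking damage it plays a timeline that drives mesh scale and circle radius, and flags whether it is the last spirit destroyed.
; After a delay for AI state to update, it shows the destroyed count on the quest HUD.
; An item-dropper reset restores scale, radius and idle motion.
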(event DamageWasSuccessfullyDealt(Damageable)
  (bind _max_number_of_evil_spirits (Variables|Default|GetMax%20Number%20Of%20Evil%20Spirits))
  (CallFunction|DyingAnimation)
  (Variables|Default|SetIm_The_Last_Evil_Spirit_Destroyed true)
  (bind _outactors (Actor|GetAllActorsOfClass "Evil_Spirit_BP_C"))
  (bind _array_element (Utilities|Array|ForEachLoopwithBreak _outactors :!label _label)
    (:LoopBody
      (if (and (not (== _array_element self)) (not (Utilities|Enum|Equal(Enum) (Variables|/Game/SpyroContent/Global_Assets/Global_Components/Base_AI_Character.Base_AI_Character_C|GetAICharacter_State (Variables|/Game/SpyroContent/Global_Assets/Global_Characters/AI_Characters/Actors/Base_AICharacter_BP.Base_AICharacter_BP_C|GetWalking_AI_Character _array_element)) "NewEnumerator3")))
        (Variables|Default|SetIm_The_Last_Evil_Spirit_Destroyed false)
        (goto _label Break)))
    (:Completed
      (bind _asspyro_player_controller (Utilities|Casting|CastToSpyro_PlayerController (Game|GetPlayerController 0)))
      ;[0 0 0 1 15] A delay is needed cause the spirit that just got killed will have it's state as "Alert" instead of "Dying"
      (Utilities|FlowControl|Delay 0.5)
      (bind _total_number_of_destroyed_spirits (CallFunction|CounttheSpirits))
      (if (Variables|Default|GetBottom%20Left%20Quest%20HUD)
        (Default|ShowBottomLeftQuestHUD _asspyro_player_controller "/Game/OT_Ports/S3/S3_Enemies/Home_00_SunriseSpring/02_CloudSpires/Evil_Spirit/Evil_Spirit_Flipbook_Mat.Evil_Spirit_Flipbook_Mat" (Utilities|String|ToString(Integer) _total_number_of_destroyed_spirits) _max_number_of_evil_spirits)
        (else
          (Default|ShowBottomRightQuestHUD _asspyro_player_controller "/Game/OT_Ports/S3/S3_Enemies/Home_00_SunriseSpring/02_CloudSpires/Evil_Spirit/Evil_Spirit_Flipbook_Mat.Evil_Spirit_Flipbook_Mat" (Utilities|String|ToString(Integer) _total_number_of_destroyed_spirits) _max_number_of_evil_spirits))))))

(event ItemDropperSuccessfullyReset(Drops_Items)
  (CallFunction|IdleAnimation)
  (Transformation|SetRelativeScale3D (Variables|Character|GetMesh) "0.125000,0.125000,0.125000")
  (Variables|Default|SetCircle%20Radius (Variables|Default|GetDefault%20Circle%20Radius)))

(event Custom|Idle%20Animation
  (bind _circle_radius (Variables|Default|GetCircle%20Radius))
  (bind (_direction _y _z) (Timeline|Idle%20Anim%20Timeline PlayFromStart)
    (:Update
      (Transformation|SetRelativeLocation (Variables|Character|GetMesh) (Math|Vector|MakeVector 0.0 (* _y _circle_radius) (* _z _circle_radius)) false false))
    (:Finished
      (CallFunction|IdleAnimation))))

(event Custom|Stop%20Idle%20Animation
  (bind _circle_radius (Variables|Default|GetCircle%20Radius))
  (bind (_direction _y _z) (Timeline|Idle%20Anim%20Timeline Stop)
    (:Update
      (Transformation|SetRelativeLocation (Variables|Character|GetMesh) (Math|Vector|MakeVector 0.0 (* _y _circle_radius) (* _z _circle_radius)) false false))
    (:Finished
      (CallFunction|IdleAnimation))))

(event Custom|Dying%20Animation
  (bind (_direction _scale _circle_radius) (Timeline|Death%20Anim%20V2%20Timeline PlayFromStart)
    (:Update
      (Transformation|SetRelativeScale3D (Variables|Character|GetMesh) (Math|Vector|MakeVector _scale _scale _scale))
      (Variables|Default|SetCircle%20Radius _circle_radius))))

(event Custom|Evil%20Spirit%20Laugh
  (if (Utilities|Enum|Equal(Enum) (Variables|/Game/SpyroContent/Global_Assets/Global_Components/Base_AI_Character.Base_AI_Character_C|GetAICharacter_State (Variables|Default|GetWalking_AI_Character)) "NewEnumerator3")
    _
    (elif (== (Math|Random|RandomIntegerinRange 0 5) 0)
      (Audio|PlaySoundatLocation "/Game/OT_Ports/S3/S3_Enemies/Home_00_SunriseSpring/02_CloudSpires/Evil_Spirit/Evil_Spirit_Laugh.Evil_Spirit_Laugh" (Transformation|GetActorLocation) "0, 0, 0" 1.0 1.0 0.0 "/Game/SpyroContent/Global_Assets/Global_Audio/Attenuation/Spyro_Attenuation_Farther.Spyro_Attenuation_Farther" 0 0)))
  (Utilities|FlowControl|Delay (Math|Random|RandomFloatinRange 4.0 6.0))
  (CallFunction|EvilSpiritLaugh))

(event EventBeginPlay
  (|CallParentFunction)
  (CallFunction|IdleAnimation)
  (Variables|Default|SetDefault%20Circle%20Radius (Variables|Default|GetCircle%20Radius))
  (Utilities|FlowControl|Delay (Math|Random|RandomFloatinRange 4.0 6.0))
  (CallFunction|EvilSpiritLaugh))

(event EventTick
  (params (DeltaSeconds :type Float%20%28single-precision%29))
  (|CallParentFunction DeltaSeconds))

(fn ConstructionScript
  (|CallParentFunction))

(fn CounttheSpirits
  (LocalVariables|SetNumber%20of%20Destroyed%20Spirits 0)
  (bind _outactors (Actor|GetAllActorsOfClass "Evil_Spirit_BP_C"))
  (for _array_element _outactors
    (if (Utilities|Enum|Equal(Enum) (Variables|/Game/SpyroContent/Global_Assets/Global_Components/Base_AI_Character.Base_AI_Character_C|GetAICharacter_State (Variables|/Game/SpyroContent/Global_Assets/Global_Characters/AI_Characters/Actors/Base_AICharacter_BP.Base_AICharacter_BP_C|GetWalking_AI_Character _array_element)) "NewEnumerator3")
      (Math|Integer|IncrementInt (LocalVariables|GetNumber%20of%20Destroyed%20Spirits))))
  (return (LocalVariables|GetNumber%20of%20Destroyed%20Spirits)))