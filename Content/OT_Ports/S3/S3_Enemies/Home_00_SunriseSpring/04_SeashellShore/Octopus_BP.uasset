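; Octopus enemy for the Seashell Shore level that combines walking and flying AI components.
; Walking AI state changes are copied to the flying AI, remove gravity while alive, restore it on Dying, and show rotating materials while Attacking.
; Melting from ice or ceasing to be afraid halts movement immediately.
; Weapon hitbox overlaps run a damage check on the other actor.
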(event OnComponentBeginOverlap(WeaponHitbox)
  (params (OverlappedComponent :type Primitive%20Component%20Object%20Reference) (OtherActor :type Actor%20Object%20Reference) (OtherComp :type Primitive%20Component%20Object%20Reference) (OtherBodyIndex :type Integer) (bFromSweep :type Boolean) (SweepResult :type Hit%20Result%20Structure%20%28by%20ref%29))
  (CallFunction|DamageCheck OtherActor OtherComp))

(event Custom|On%20State%20Change
  (bind _mesh (Variables|Character|GetMesh))
  (bind _walking_ai_character (Variables|Default|GetWalking_AI_Character))
  (bind _charactermovement (Variables|Character|GetCharacterMovement))
  (bind _aicharacter_state (Variables|/Game/SpyroContent/Global_Assets/Global_Components/Base_AI_Character.Base_AI_Character_C|GetAICharacter_State _walking_ai_character))
  (Default|ChangeAICharacterState (Variables|Default|GetFlying_AI_Character) _aicharacter_state)
  (switch Utilities|FlowControl|Switch|SwitchonAICharacter_States _aicharacter_state
    (:NewEnumerator0
      (Variables|/Script/Engine.CharacterMovementComponent|SetGravityScale _charactermovement 0.0 :!label _label))
    (:NewEnumerator1
      (goto _label))
    (:NewEnumerator2
      (goto _label))
    (:NewEnumerator3
      (Variables|/Script/Engine.CharacterMovementComponent|SetGravityScale _charactermovement 1.5)))
  (switch Utilities|FlowControl|Switch|SwitchonAICharacter_States _aicharacter_state
    (:NewEnumerator0
      (Rendering|Material|SetMaterial _mesh 0 (Variables|Default|GetUntex%20Material%20Normal) :!label _label_2)
      (Rendering|Material|SetMaterial _mesh 1 (Variables|Default|GetTex%20Material%20Normal)))
    (:NewEnumerator1
      (goto _label_2))
    (:NewEnumerator2
      (Rendering|Material|SetMaterial _mesh 0 (Variables|Default|GetUntex%20Material%20Rotating))
      (Rendering|Material|SetMaterial _mesh 1 (Variables|Default|GetTex%20Material%20Rotating)))
    (:NewEnumerator3
      (goto _label_2))))

(event Custom|Character%20melted
  (Components|Movement|StopMovementImmediately (Variables|Character|GetCharacterMovement)))

(event EventBeginPlay
  (|CallParentFunction)
  (EventDispatchers|BindEventtoMyStateChanged (Variables|Default|GetWalking_AI_Character) (delegate Custom|On%20State%20Change))
  (EventDispatchers|BindEventtoMeltedfromIce (Variables|Default|GetDamageable) (delegate Custom|Character%20melted))
  (EventDispatchers|BindEventtoCallStopBeingAfraid (Variables|Default|GetDamageable) (delegate Custom|Character%20melted)))

(event Collision|EventActorBeginOverlap
  (params (OtherActor :type Actor%20Object%20Reference)))

(event EventTick
  (params (DeltaSeconds :type Float%20%28single-precision%29))
  (|CallParentFunction DeltaSeconds) ; This node is disabled and will not be called.\nDrag off pins to build functionality.
)

(fn ConstructionScript
  (|CallParentFunction))