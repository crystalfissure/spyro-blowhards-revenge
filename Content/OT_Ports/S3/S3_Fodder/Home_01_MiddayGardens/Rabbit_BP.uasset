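; Rabbit actor for the Midday Gardens home level that adds occasional ambient rabbit sounds on top of its parent class.
; From BeginPlay, a self-calling event loops on a short random delay, with a random chance each pass to play the sound at the rabbit's location.
; Playback is skipped while the WalkingAICharacter is in one particular AI state.
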(event Custom|Rabbit%20SFX
  (if (== (Math|Random|RandomIntegerinRange 0 5) 0)
    (if (Utilities|Enum|NotEqual(Enum) (Variables|/Game/SpyroContent/Global_Assets/Global_Components/Base_AI_Character.Base_AI_Character_C|GetAICharacter_State (Variables|Default|GetWalking_AI_Character)) "NewEnumerator3")
      (Audio|PlaySoundatLocation "/Game/OT_Ports/S3/S3_Fodder/Home_01_MiddayGardens/Rabbit/Rabbit_SFX.Rabbit_SFX" (Transformation|GetActorLocation) "0, 0, 0" 1.0 1.0 0.0 "/Game/SpyroContent/Global_Assets/Global_Audio/Attenuation/Spyro_Attenuation.Spyro_Attenuation" 0 0)))
  (Utilities|FlowControl|Delay (Math|Random|RandomFloatinRange 1.0 3.0))
  (CallFunction|RabbitSFX))

(event EventBeginPlay
  (|CallParentFunction)
  (Utilities|FlowControl|Delay (Math|Random|RandomFloatinRange 1.0 3.0))
  (CallFunction|RabbitSFX))

(event Collision|EventActorBeginOverlap
  (params (OtherActor :type Actor%20Object%20Reference)))

(event EventTick
  (params (DeltaSeconds :type Float%20%28single-precision%29)))

(fn ConstructionScript
  (|CallParentFunction))