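; Cactus Blueprint for the Peace Keepers Dry Canyon level that wobbles when damaged and chars temporarily under one specific damage type.
; Damage triggers a timeline-driven pitch wobble, with DoOnce gates blocking retriggers until it finishes.
; A burn timeline drives the dynamic material's ColorChange parameter.
; After wobbling, a burned cactus reverses that color, plays a shake animation, spawns a Basket_Burst_BP shard burst, then returns to idle.
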(event Custom|Cactus%20Damaged
  (Utilities|FlowControl|DoOnce false
    (:Completed
      (if (Utilities|Enum|Equal(Enum) (Variables|/Game/SpyroContent/Global_Assets/Global_Components/Damageable_Com.Damageable_Com_C|GetDeal%20Damage%20-%20Damage%20Type (Variables|Default|GetDamageable)) "NewEnumerator1")
        (Variables|Default|SetBurned true)
        (CallFunction|Burn))
      (CallFunction|Wobble))))

(event Custom|Wobble
  (Utilities|FlowControl|DoOnce false
    (:Completed
      (Variables|Default|SetDone%20wobbling false)
      (bind _newtrack_0 (Timeline|Timeline_1 PlayFromStart)
        (:Update
          (Transformation|SetRelativeRotation (Variables|Character|GetMesh) (Math|Rotator|MakeRotator 9e+01 _newtrack_0 0.0) false false))
        (:Finished
          (if (Variables|Default|GetBurned)
            (Utilities|FlowControl|Delay 0.5)
            (CallFunction|Un-Burn)
            (Components|Animation|PlayAnimation (Variables|Character|GetMesh) (Variables|Default|GetAnim%20Shake) false)
            (bind _returnvalue (Game|SpawnActorfromClass "/Game/SpyroContent/Global_Assets/Global_Level_Items/Treasure_Containers/Basket/Actors/Basket_Burst_BP.Basket_Burst_BP_C" (Transformation|GetWorldTransform (Variables|Default|GetProjectile%20Spawn%20Location)) "Undefined" 0 0))
            (Default|ShardBurstAction _returnvalue "/Game/OT_Ports/S1/S1_Objects/Home_01_Peace_Keepers/01_DryCanyon/Cactuses/Cactus_Particles.Cactus_Particles" "/Game/OT_Ports/S1/S1_Objects/Home_01_Peace_Keepers/01_DryCanyon/Cactuses/Cactus_Particles.Cactus_Particles")
            (Utilities|FlowControl|Delay 1.25)
            (Variables|Default|SetBurned false)
            (Components|Animation|PlayAnimation (Variables|Character|GetMesh) (Variables|Default|GetAnim%20Idle) false))
          (CallFunction|CanDealDamageAgain)
          (Variables|Default|SetDone%20wobbling true)
          (CallFunction|CanWobbleAgain))))))

(event Custom|Burn
  (bind _newtrack_1 (Timeline|Burn%20effect PlayFromStart)
    (:Update
      (Rendering|Material|SetVectorParameterValue (Variables|Default|GetDynMat) "ColorChange" (Utilities|Struct|MakeLinearColor _newtrack_1 _newtrack_1 _newtrack_1 1.0) :!class /Script/Engine.MaterialInstanceDynamic))))

(event Custom|Un-Burn
  (bind _newtrack_1 (Timeline|Burn%20effect ReverseFromEnd)
    (:Update
      (Rendering|Material|SetVectorParameterValue (Variables|Default|GetDynMat) "ColorChange" (Utilities|Struct|MakeLinearColor _newtrack_1 _newtrack_1 _newtrack_1 1.0) :!class /Script/Engine.MaterialInstanceDynamic))))

(event Custom|Can%20Deal%20Damage%20Again
  (Utilities|FlowControl|DoOnce false) ; enters at Reset
)

(event Custom|Can%20Wobble%20Again
  (Utilities|FlowControl|DoOnce false) ; enters at Reset
)

(event EventBeginPlay
  (|CallParentFunction)
  (bind _returnvalue (Rendering|Material|CreateDynamicMaterialInstance (Variables|Character|GetMesh) 0 (Rendering|Material|GetMaterial (Variables|Character|GetMesh) 0) "None" :!class /Script/Engine.PrimitiveComponent))
  (Variables|Default|SetDynMat _returnvalue)
  (EventDispatchers|BindEventtoCallDealDamage (Variables|Default|GetDamageable) (delegate Custom|Cactus%20Damaged)))

(event EventResetThisAICharacter)

(fn ConstructionScript
  (|CallParentFunction))