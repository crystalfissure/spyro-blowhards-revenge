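; Cauldron treasure container for the Cliff Town object set, holding an Acid component that damages players who hit it.
; A hit on Acid deals damage through the playable character's Damageable, only when the capsule is the component struck.
; Successfully damaging the container hides the acid and disables its collision; a reset restores both unless the container is destroyed.
; The parent's spring chest material setup is overridden to do nothing.
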(event OnComponentHit(Acid)
  (params (HitComponent :type Primitive%20Component%20Object%20Reference) (OtherActor :type Actor%20Object%20Reference) (OtherComp :type Primitive%20Component%20Object%20Reference) (NormalImpulse :type Vector :default "0, 0, 0") (Hit :type Hit%20Result%20Structure%20%28by%20ref%29))
  (bind _asbp_base_playable (Utilities|Casting|CastToBP_Base_Playable OtherActor))
  (if (== (Variables|/Script/Engine.Character|GetCapsuleComponent _asbp_base_playable) OtherComp)
    (Default|DealDamage (Variables|/Game/SpyroContent/Global_Assets/Global_Characters/Playable_Characters/BP_Base_Playable.BP_Base_Playable_C|GetDamageable _asbp_base_playable) "NewEnumerator1" "0, 0, 0" false 0 false)))

(event EventBeginPlay
  (|CallParentFunction) ; This node is disabled and will not be called.\nDrag off pins to build functionality.
)

(event EventTreasureContainerSuccessfullyDamaged
  (bind _acid (Variables|Default|GetAcid))
  (|CallParentFunction)
  (Rendering|SetVisibility _acid false false)
  (Collision|SetCollisionEnabled _acid "NoCollision"))

(event EventTick
  (params (DeltaSeconds :type Float%20%28single-precision%29)))

(event Collision|EventActorBeginOverlap
  (params (OtherActor :type Actor%20Object%20Reference)))

(event EventResetThisContainer
  (bind _acid (Variables|Default|GetAcid))
  (|CallParentFunction)
  (if (not (Variables|Default|GetContainer_Destroyed))
    (Rendering|SetVisibility _acid true false)
    (Collision|SetCollisionEnabled _acid "QueryAndPhysics")))

(fn ConstructionScript
  (|CallParentFunction))

(fn SetSpringChestMat)