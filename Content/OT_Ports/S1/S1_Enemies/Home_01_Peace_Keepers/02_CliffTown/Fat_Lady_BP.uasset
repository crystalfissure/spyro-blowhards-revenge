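; Fat Lady enemy Blueprint for the Peace Keepers Cliff Town area, whose weapon hit launches characters.
; On weapon hitbox overlap, it checks for another actor's damageable hitbox, a specific AI state, and that she is neither frozen nor fear-paralyzed.
; A valid hit launches the Character along her forward vector plus an upward boost, overriding velocity.
; For playable characters, it also changes the player state and sets her laughing flag.
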(event OnComponentBeginOverlap(WeaponHitbox)
  (params (OverlappedComponent :type Primitive%20Component%20Object%20Reference) (OtherActor :type Actor%20Object%20Reference) (OtherComp :type Primitive%20Component%20Object%20Reference) (OtherBodyIndex :type Integer) (bFromSweep :type Boolean) (SweepResult :type Hit%20Result%20Structure%20%28by%20ref%29))
  (bind _returnvalue (Transformation|GetActorForwardVector))
  (bind _launch_forward_velocity (Variables|Default|GetLaunch%20Forward%20Velocity))
  (bind _damageable (Variables|Default|GetDamageable))
  (bind _returnvalue_2 (* _returnvalue _launch_forward_velocity))
  (if (Math|Boolean|ANDBoolean (== (Variables|/Game/SpyroContent/Global_Assets/Global_Components/Damageable_Com.Damageable_Com_C|GetObject's%20Hitbox%20Component (Actor|GetComponentbyClass OtherActor "/Game/SpyroContent/Global_Assets/Global_Components/Damageable_Com.Damageable_Com_C")) OtherComp) (not (== self OtherActor)) (Utilities|Enum|Equal(Enum) (Variables|/Game/SpyroContent/Global_Assets/Global_Components/Base_AI_Character.Base_AI_Character_C|GetAICharacter_State (Variables|Default|GetWalking_AI_Character)) "NewEnumerator2") (not (Variables|/Game/SpyroContent/Global_Assets/Global_Components/Damageable_Com.Damageable_Com_C|GetFrozen _damageable)) (not (Variables|/Game/SpyroContent/Global_Assets/Global_Components/Damageable_Com.Damageable_Com_C|GetParalyzed_by_Fear _damageable)))
    (bind _ascharacter (Utilities|Casting|CastToCharacter OtherActor))
    (Character|LaunchCharacter _ascharacter (Math|Vector|MakeVector (.x _returnvalue_2) (.y _returnvalue_2) (+ (.z _returnvalue_2) (Variables|Default|GetLaunch%20Updwards%20Velocity))) true true)
    (bind _asbp_base_playable (Utilities|Casting|CastToBP_Base_Playable OtherActor))
    (Variables|/Game/SpyroContent/Global_Assets/Global_Characters/Playable_Characters/BP_Base_Playable.BP_Base_Playable_C|SetPlayer_State _asbp_base_playable "NewEnumerator10")
    (Variables|Default|SetisLaughing true)))

(event EventBeginPlay
  (|CallParentFunction) ; This node is disabled and will not be called.\nDrag off pins to build functionality.
)

(event Collision|EventActorBeginOverlap
  (params (OtherActor :type Actor%20Object%20Reference)))

(event EventTick
  (params (DeltaSeconds :type Float%20%28single-precision%29))
  (|CallParentFunction DeltaSeconds) ; This node is disabled and will not be called.\nDrag off pins to build functionality.
)

(fn ConstructionScript
  (|CallParentFunction))