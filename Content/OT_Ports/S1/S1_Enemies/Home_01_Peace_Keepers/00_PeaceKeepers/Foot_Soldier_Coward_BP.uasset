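; Foot Soldier Coward, a Peace Keeper enemy Blueprint that builds on an inherited parent class.
; On BeginPlay it runs the parent logic, then sizes the alert sphere and a larger unalert sphere from a shared AlertRadiusScale.
; Tick and construction only forward to the parent, so any cowardly behavior lives outside these graphs.
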(event EventBeginPlay
  (bind _alert_radius_scale (Variables|Default|GetAlert%20Radius%20Scale))
  (|CallParentFunction)
  (Components|Sphere|SetSphereRadius (Variables|Default|GetAlert_Radius) (* 6e+02 _alert_radius_scale) true)
  (Components|Sphere|SetSphereRadius (Variables|Default|GetUnalert_Radius) (* 7.5e+02 _alert_radius_scale) true))

(event Collision|EventActorBeginOverlap
  (params (OtherActor :type Actor%20Object%20Reference)))

(event EventTick
  (params (DeltaSeconds :type Float%20%28single-precision%29))
  (|CallParentFunction DeltaSeconds))

(fn ConstructionScript
  (|CallParentFunction))