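; Projectile Blueprint for the Gnorc Muskeeter enemy's musket, defining how the shot explodes.
; InvokedBlowUp runs once, hiding the mesh and trail particles, playing blast effects and impact sound, and starting a delayed self-destruct.
; A zero-length multi-sphere trace acts as the blast radius, passing each hit to DamageImpactTarget and spawning a Basket_Burst_BP debris burst per hit.
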(event EventBeginPlay
  (|CallParentFunction) ; This node is disabled and will not be called.\nDrag off pins to build functionality.
)

(event Collision|EventActorBeginOverlap
  (params (OtherActor :type Actor%20Object%20Reference)))

(event EventTick
  (params (DeltaSeconds :type Float%20%28single-precision%29))
  (|CallParentFunction DeltaSeconds) ; This node is disabled and will not be called.\nDrag off pins to build functionality.
)

(event EventInvokedBlowUp
  (bind _returnvalue (Transformation|GetActorLocation))
  (bind _returnvalue_2 (Transformation|GetActorLocation))
  (Utilities|FlowControl|DoOnce false
    (:Completed
      (Variables|Default|SetBlowing_Up true)
      (Components|Activation|Deactivate (Variables|Default|GetParticleSystem))
      (Rendering|SetVisibility (Variables|Default|GetStaticMesh) false false)
      (CallFunction|DelayedSelfDestruct (Variables|Default|GetExplosion%20Duration))
      (Effects|SpawnEmitteratLocation (Variables|Default|GetBlast_Type) _returnvalue (Math|Rotator|MakeRotator 0.0 0.0 (- (.yaw (Transformation|GetWorldRotation (Variables|Default|GetStaticMesh))) 9e+01)))
      (Audio|PlaySoundatLocation (Variables|Default|GetImpact%20SFX) _returnvalue "0, 0, 0" 1.0 1.0 0.0 0 0 0)
      (bind _outhits (Collision|MultiSphereTraceForObjects _returnvalue_2 _returnvalue_2 (Variables|Default|GetExplosion%20Radius) (Utilities|Array|MakeArray "ObjectTypeQuery1" "ObjectTypeQuery2" "ObjectTypeQuery3" "ObjectTypeQuery8" "ObjectTypeQuery9") false 0 "None"))
      (for _array_element _outhits
        (CallFunction|DamageImpactTarget (.hitactor _array_element) (.hitcomponent _array_element))
        (bind _returnvalue_3 (Game|SpawnActorfromClass "/Game/SpyroContent/Global_Assets/Global_Level_Items/Treasure_Containers/Basket/Actors/Basket_Burst_BP.Basket_Burst_BP_C" (Transformation|GetActorTransform) "Undefined" 0 0))
        (Default|ShardBurstAction _returnvalue_3 "/Game/OT_Ports/S1/S1_Enemies/Home_01_Peace_Keepers/01_DryCanyon/Gnorc_Muskeeter/Projectile/Musket_Projectile_Debris.Musket_Projectile_Debris" "/Game/OT_Ports/S1/S1_Enemies/Home_01_Peace_Keepers/01_DryCanyon/Gnorc_Muskeeter/Projectile/Musket_Projectile_Debris.Musket_Projectile_Debris")))))

(fn ConstructionScript
  (|CallParentFunction))