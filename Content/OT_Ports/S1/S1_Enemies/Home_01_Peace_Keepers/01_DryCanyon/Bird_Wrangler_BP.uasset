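; Bird Wrangler enemy Blueprint for the Dry Canyon level of the Peace Keepers home world.
; On BeginPlay it binds to its WalkingAICharacter's state change and spawns Bird_Wrangler_Death_BP at its transform when the state becomes Dying.
; Overlaps on its weapon hitbox are passed to DamageCheck to handle hits on other actors.
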(event OnComponentBeginOverlap(WeaponHitbox)
  (params (OverlappedComponent :type Primitive%20Component%20Object%20Reference) (OtherActor :type Actor%20Object%20Reference) (OtherComp :type Primitive%20Component%20Object%20Reference) (OtherBodyIndex :type Integer) (bFromSweep :type Boolean) (SweepResult :type Hit%20Result%20Structure%20%28by%20ref%29))
  (CallFunction|DamageCheck OtherActor OtherComp))

(event Custom|Hedge%20State%20Changed
  (switch Utilities|FlowControl|Switch|SwitchonAICharacter_States (Variables|/Game/SpyroContent/Global_Assets/Global_Components/Base_AI_Character.Base_AI_Character_C|GetAICharacter_State (Variables|Default|GetWalking_AI_Character))
    (:NewEnumerator3
      (Game|SpawnActorfromClass "/Game/OT_Ports/S1/S1_Enemies/Home_01_Peace_Keepers/01_DryCanyon/Bird_Wrangler/Bird_Wrangler_Death_BP.Bird_Wrangler_Death_BP_C" (Transformation|GetActorTransform) "AlwaysSpawn" 0 0))))

(event EventBeginPlay
  (|CallParentFunction)
  (EventDispatchers|BindEventtoMyStateChanged (Variables|Default|GetWalking_AI_Character) (delegate Custom|Hedge%20State%20Changed)))

(event Collision|EventActorBeginOverlap
  (params (OtherActor :type Actor%20Object%20Reference)))

(event EventTick
  (params (DeltaSeconds :type Float%20%28single-precision%29))
  (|CallParentFunction DeltaSeconds) ; This node is disabled and will not be called.\nDrag off pins to build functionality.
)

(fn ConstructionScript
  (|CallParentFunction))