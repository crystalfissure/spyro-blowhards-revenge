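; Gnorc Soldier enemy Blueprint for Dark Hollow, built on a walking AI character with a shield and a weapon.
; Weapon hitbox overlaps feed a damage check, while BeginPlay registers the shield hitbox and the metal-material mesh with the Damageable component.
; AI state changes toggle shield collision: it is on in Alert and off when Idle, Attacking or Dying.
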(event OnComponentBeginOverlap(WeaponHitbox)
  (params (OverlappedComponent :type Primitive%20Component%20Object%20Reference) (OtherActor :type Actor%20Object%20Reference) (OtherComp :type Primitive%20Component%20Object%20Reference) (OtherBodyIndex :type Integer) (bFromSweep :type Boolean) (SweepResult :type Hit%20Result%20Structure%20%28by%20ref%29))
  (CallFunction|DamageCheck OtherActor OtherComp))

(event Custom|On%20Pony%20State%20Changed
  (bind _shield_hitbox (Variables|Default|GetShield%20Hitbox))
  (switch Utilities|FlowControl|Switch|SwitchonAICharacter_States (Variables|/Game/SpyroContent/Global_Assets/Global_Components/Base_AI_Character.Base_AI_Character_C|GetAICharacter_State (Variables|Default|GetWalking_AI_Character))
    (:NewEnumerator0
      (Collision|SetCollisionEnabled _shield_hitbox "NoCollision" :!label _label))
    (:NewEnumerator1
      (Collision|SetCollisionEnabled _shield_hitbox "QueryAndPhysics"))
    (:NewEnumerator2
      (goto _label))
    (:NewEnumerator3
      (goto _label))))

(event EventBeginPlay
  (|CallParentFunction)
  (EventDispatchers|BindEventtoMyStateChanged (Variables|Default|GetWalking_AI_Character) (delegate Custom|On%20Pony%20State%20Changed))
  (Variables|/Game/SpyroContent/Global_Assets/Global_Components/Damageable_Com.Damageable_Com_C|SetObject's%20Shield%20Component (Variables|Default|GetDamageable) (Variables|Default|GetShield%20Hitbox))
  (Variables|/Game/SpyroContent/Global_Assets/Global_Components/Damageable_Com.Damageable_Com_C|SetComponent_with_Metal_Material (Variables|Default|GetDamageable) (Variables|Character|GetMesh)))

(event Collision|EventActorBeginOverlap
  (params (OtherActor :type Actor%20Object%20Reference)))

(event EventTick
  (params (DeltaSeconds :type Float%20%28single-precision%29))
  (|CallParentFunction DeltaSeconds) ; This node is disabled and will not be called.\nDrag off pins to build functionality.
)

(fn ConstructionScript
  (|CallParentFunction))