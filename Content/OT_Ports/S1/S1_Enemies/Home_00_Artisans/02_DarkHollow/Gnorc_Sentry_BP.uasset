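; Gnorc Sentry enemy for Dark Hollow that patrols between its spawn and a MoveTo point, pausing to attack or laugh.
; Its belly hit launches the player away without dealing damage, as the DealDamage call is disconnected.
; Front and rear detection volumes swap sides each leg, switching damage resistances by the player's side, and an optional headbash hitbox deals super damage.
; Attack cooldown, radius and delay scale with difficulty, including skill-based Dynamic mode.
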(event OnComponentBeginOverlap(BellyHitbox)
  (params (OverlappedComponent :type Primitive%20Component%20Object%20Reference) (OtherActor :type Actor%20Object%20Reference) (OtherComp :type Primitive%20Component%20Object%20Reference) (OtherBodyIndex :type Integer) (bFromSweep :type Boolean) (SweepResult :type Hit%20Result%20Structure%20%28by%20ref%29))
  (CallFunction|DamageCheck OtherActor OtherComp))

(event OnComponentBeginOverlap(Headbash_Hitbox)
  (params (OverlappedComponent :type Primitive%20Component%20Object%20Reference) (OtherActor :type Actor%20Object%20Reference) (OtherComp :type Primitive%20Component%20Object%20Reference) (OtherBodyIndex :type Integer) (bFromSweep :type Boolean) (SweepResult :type Hit%20Result%20Structure%20%28by%20ref%29))
  (if (Variables|Default|GetCan%20be%20Headbashed)
    (bind _asbp_base_playable (Utilities|Casting|CastToBP_Base_Playable OtherActor))
    (if (and (Utilities|Enum|Equal(Enum) (Variables|/Game/SpyroContent/Global_Assets/Global_Characters/Playable_Characters/BP_Base_Playable.BP_Base_Playable_C|GetPlayer_State _asbp_base_playable) "NewEnumerator8") (== (Variables|/Script/Engine.Character|GetCapsuleComponent _asbp_base_playable) OtherComp))
      (Default|DealDamage (Variables|Default|GetDamageable) "NewEnumerator2" "0, 0, 0" true _asbp_base_playable false))))

(event DamageWasSuccessfullyDealt(Damageable)
  (bind _mesh (Variables|Character|GetMesh))
  (bind _returnvalue (Transformation|GetRelativeTransform _mesh))
  (bind _rotation (Math|Transform|BreakTransform _returnvalue))
  (bind (_roll _pitch _yaw) (Math|Rotator|BreakRotator _rotation))
  (if (Variables|Default|GetMovingToEnd)
    (Transformation|SetRelativeRotation (Variables|Character|GetMesh) (Math|Rotator|MakeRotator _roll _pitch (+ _yaw 1.8e+02)) false false))
  (Variables|Default|SetisDying true))

(event OnComponentBeginOverlap(NotFacingSpyroDetection)
  (params (OverlappedComponent :type Primitive%20Component%20Object%20Reference) (OtherActor :type Actor%20Object%20Reference) (OtherComp :type Primitive%20Component%20Object%20Reference) (OtherBodyIndex :type Integer) (bFromSweep :type Boolean) (SweepResult :type Hit%20Result%20Structure%20%28by%20ref%29))
  (bind _asbp_base_playable (Utilities|Casting|CastToBP_Base_Playable OtherActor))
  (if (== (Variables|/Script/Engine.Character|GetCapsuleComponent _asbp_base_playable) OtherComp)
    (Variables|/Game/SpyroContent/Global_Assets/Global_Components/Damageable_Com.Damageable_Com_C|SetDamage_Resistances (Variables|Default|GetDamageable) (Variables|Default|GetDamage%20Resists%20While%20Not%20Facing%20Spyro))))

(event ItemDropperSuccessfullyReset(Drops_Items)
  (bind _initial_rotation (Variables|Default|GetInitial%20Rotation))
  (bind (_roll _pitch _yaw) (Math|Rotator|BreakRotator _initial_rotation))
  (if (Variables|Default|GetisDying)
    (Variables|Default|SetisDying false)
    (Transformation|SetRelativeScale3D (Variables|Character|GetMesh) (Variables|Default|GetInital%20Scale))
    (Transformation|SetRelativeRotation (Variables|Default|GetCapsuleComponent) (Variables|Default|GetInitial%20Capsule%20Rotation) false false)
    (if (Variables|Default|GetRotateMeshAfterReachingEndPoint)
      (if (Variables|Default|GetMovingToEnd)
        (Transformation|SetRelativeRotation (Variables|Character|GetMesh) _initial_rotation false false)
        (else
          (Transformation|SetRelativeRotation (Variables|Character|GetMesh) (Math|Rotator|MakeRotator _roll _pitch (+ _yaw 1.8e+02)) false false))))))

(event OnComponentBeginOverlap(FacingSpyroDetection)
  (params (OverlappedComponent :type Primitive%20Component%20Object%20Reference) (OtherActor :type Actor%20Object%20Reference) (OtherComp :type Primitive%20Component%20Object%20Reference) (OtherBodyIndex :type Integer) (bFromSweep :type Boolean) (SweepResult :type Hit%20Result%20Structure%20%28by%20ref%29))
  (bind _asbp_base_playable (Utilities|Casting|CastToBP_Base_Playable OtherActor))
  (if (== (Variables|/Script/Engine.Character|GetCapsuleComponent _asbp_base_playable) OtherComp)
    (Variables|/Game/SpyroContent/Global_Assets/Global_Components/Damageable_Com.Damageable_Com_C|SetDamage_Resistances (Variables|Default|GetDamageable) (Variables|Default|GetDamage%20Resists%20While%20Facing%20Spyro))))

(event Custom|On%20Pony%20State%20Changed
  (bind _shield_hitbox (Variables|Default|GetShield%20Hitbox))
  (switch Utilities|FlowControl|Switch|SwitchonAICharacter_States (Variables|/Game/SpyroContent/Global_Assets/Global_Components/Base_AI_Character.Base_AI_Character_C|GetAICharacter_State (Variables|Default|GetWalking_AI_Character))
    (:NewEnumerator0
      (Collision|SetCollisionEnabled _shield_hitbox "QueryAndPhysics" :!label _label))
    (:NewEnumerator1
      (goto _label))
    (:NewEnumerator2
      (goto _label))
    (:NewEnumerator3
      (Collision|SetCollisionEnabled _shield_hitbox "NoCollision"))))

(event Custom|Damage%20Check
  (params (Other%20Actor :type Actor%20Object%20Reference) (Other%20Comp :type Primitive%20Component%20Object%20Reference))
  (bind _damageable (Variables|Default|GetDamageable))
  (if (Math|Boolean|ANDBoolean (== (Variables|/Game/SpyroContent/Global_Assets/Global_Components/Damageable_Com.Damageable_Com_C|GetObject's%20Hitbox%20Component (Actor|GetComponentbyClass Other%20Actor "/Game/SpyroContent/Global_Assets/Global_Components/Damageable_Com.Damageable_Com_C")) Other%20Comp) (not (== self Other%20Actor)) (Utilities|Enum|Equal(Enum) (Variables|/Game/SpyroContent/Global_Assets/Global_Components/Base_AI_Character.Base_AI_Character_C|GetAICharacter_State (Variables|Default|GetWalking_AI_Character)) "NewEnumerator2") (not (Variables|/Game/SpyroContent/Global_Assets/Global_Components/Damageable_Com.Damageable_Com_C|GetFrozen _damageable)) (not (Variables|/Game/SpyroContent/Global_Assets/Global_Components/Damageable_Com.Damageable_Com_C|GetParalyzed_by_Fear _damageable)))
    (bind _asbp_base_playable (Utilities|Casting|CastToBP_Base_Playable Other%20Actor)
      (:then
        (if (not (Utilities|Enum|Equal(Enum) (Variables|/Game/SpyroContent/Global_Assets/Global_Characters/Playable_Characters/BP_Base_Playable.BP_Base_Playable_C|GetPlayer_State _asbp_base_playable) "NewEnumerator8"))
          (if (not (Variables|/Game/SpyroContent/Global_Assets/Global_Components/Damageable_Com.Damageable_Com_C|GetParalyzed_by_Fear (Variables|/Game/SpyroContent/Global_Assets/Global_Characters/Playable_Characters/BP_Base_Playable.BP_Base_Playable_C|GetDamageable _asbp_base_playable)))
            (CallFunction|LaunchSpyro _asbp_base_playable :!label _label)
            (if (Variables|Default|GetLaughs%20After%20Successfull%20Attack)
              (Variables|Default|SetisLaughing true)))))
      (:CastFailed
        (goto _label)))))

(event Custom|Launch%20Spyro
  (params (BP%20Base%20Playable%20Ref :type Actor%20Object%20Reference))
  (bind _launch_forward_velocity (Variables|Default|GetLaunch%20Forward%20Velocity))
  (bind _mesh (Variables|Character|GetMesh))
  (bind _returnvalue (Transformation|GetWorldRotation _mesh))
  (bind _returnvalue_2 (Math|Vector|GetForwardVector _returnvalue))
  (bind _returnvalue_3 (Math|Vector|RotateVector _returnvalue_2 "0,90.000000, 0"))
  (bind _returnvalue_4 (* _returnvalue_3 _launch_forward_velocity))
  (bind _ascharacter (Utilities|Casting|CastToCharacter BP%20Base%20Playable%20Ref))
  (Character|LaunchCharacter _ascharacter (Math|Vector|MakeVector (.x _returnvalue_4) (.y _returnvalue_4) (+ (.z _returnvalue_4) (Variables|Default|GetLaunch%20Updwards%20Velocity))) true true)
  (bind _asbp_base_playable (Utilities|Casting|CastToBP_Base_Playable BP%20Base%20Playable%20Ref))
  (Variables|/Game/SpyroContent/Global_Assets/Global_Characters/Playable_Characters/BP_Base_Playable.BP_Base_Playable_C|SetPlayer_State _asbp_base_playable "NewEnumerator10")
  (Variables|Default|SetisLaughing true))

(event EventTick
  (params (DeltaSeconds :type Float%20%28single-precision%29))
  (bind _mesh (Variables|Character|GetMesh))
  (bind _attack_radius (Variables|Default|GetAttack_Radius))
  (bind _facing_spyro_detection (Variables|Default|GetFacing%20Spyro%20Detection))
  (bind _not_facing_spyro_detection (Variables|Default|GetNot%20Facing%20Spyro%20Detection))
  (bind _returnvalue (Transformation|GetRelativeTransform _mesh))
  (bind _rotation (Math|Transform|BreakTransform _returnvalue))
  (bind (_roll _pitch _yaw) (Math|Rotator|BreakRotator _rotation))
  (if (not (Variables|Default|GetisDying))
    (if (not (Utilities|Enum|Equal(Enum) (Variables|/Game/SpyroContent/Global_Assets/Global_Components/Base_AI_Character.Base_AI_Character_C|GetAICharacter_State (Variables|Default|GetWalking_AI_Character)) "NewEnumerator2"))
      (if (not (Variables|Default|GetisLaughing))
        (Transformation|AddActorWorldOffset (* (Math|Vector|Normalize (- (Variables|Default|GetCurrentTarget) (Transformation|GetActorLocation))) (* (Variables|Default|GetMove%20Speed) (Utilities|Time|GetWorldDeltaSeconds))))
        (if (Variables|Default|GetMovingToEnd)
          (if (Math|Vector|Equal(Vector) (Variables|Default|GetEndPoint) (Transformation|GetActorLocation) 1e+02)
            (Variables|Default|SetMovingToEnd false)
            (Variables|Default|SetCurrentTarget (Variables|Default|GetStartPoint))
            (Transformation|SetRelativeLocation _attack_radius "-135.000000, 0, 0" false false)
            (Transformation|SetRelativeLocation _facing_spyro_detection "-320.000000, 0, 0" false false)
            (Transformation|SetRelativeLocation _not_facing_spyro_detection "320.000000, 0, 0" false false)
            (if (Variables|Default|GetRotateMeshAfterReachingEndPoint) :!label _label
              (Transformation|SetRelativeRotation (Variables|Character|GetMesh) (Math|Rotator|MakeRotator _roll _pitch (+ _yaw 1.8e+02)) false false)))
          (elif (Math|Vector|Equal(Vector) (Variables|Default|GetStartPoint) (Transformation|GetActorLocation) 1e+02)
            (Variables|Default|SetMovingToEnd true)
            (Variables|Default|SetCurrentTarget (Variables|Default|GetEndPoint))
            (Transformation|SetRelativeLocation _attack_radius "135.000000, 0, 0" false false)
            (Transformation|SetRelativeLocation _facing_spyro_detection "320.000000, 0, 0" false false)
            (Transformation|SetRelativeLocation _not_facing_spyro_detection "-320.000000, 0, 0" false false)
            (goto _label)))))))

(event EventSetMyDifficulty
  (bind _easy_attack_delay (Variables|Difficulty|GetEasy%20Attack%20Delay))
  (bind _nightmare_attack_delay (Variables|Difficulty|GetNightmare%20Attack%20Delay))
  (bind _hard_attack_radius (Variables|Difficulty|GetHard%20Attack%20Radius))
  (bind _hard_attack_delay (Variables|Difficulty|GetHard%20Attack%20Delay))
  (bind _medium_attack_delay (Variables|Difficulty|GetMedium%20Attack%20Delay))
  (bind _easy_attack_radius (Variables|Difficulty|GetEasy%20Attack%20Radius))
  (bind _medium_attack_radius (Variables|Difficulty|GetMedium%20Attack%20Radius))
  (bind _nightmare_attack_radius (Variables|Difficulty|GetNightmare%20Attack%20Radius))
  (bind _easy_max_attack_cooldown (Variables|Difficulty|GetEasy%20Max%20Attack%20Cooldown))
  (bind _medium_max_attack_cooldown (Variables|Difficulty|GetMedium%20Max%20Attack%20Cooldown))
  (bind _nightmare_max_attack_cooldown (Variables|Difficulty|GetNightmare%20Max%20Attack%20Cooldown))
  (bind _hard_max_attack_cooldown (Variables|Difficulty|GetHard%20Max%20Attack%20Cooldown))
  (|CallParentFunction)
  (bind _asspyro_universal_save_data (CallFunction|LoadUniversalSave))
  (if (Utilities|Enum|Equal(Enum) (Variables|/Game/SpyroContent/Global_Assets/Global_SaveData/Spyro_Universal_Save_Data.Spyro_Universal_Save_Data_C|GetDifficulty _asspyro_universal_save_data) "NewEnumerator4")
    (bind _asspyro_save_data (CallFunction|LoadSpyroGame self))
    (bind _difficulty (CallFunction|ConvertSkillLevelFloattoEnum (Variables|/Game/SpyroContent/Global_Assets/Global_SaveData/Spyro_SaveData.Spyro_SaveData_C|GetSkill_Level _asspyro_save_data)))
    (Variables|Default|SetMax_Attack_Cooldown (Utilities|Select :Index _difficulty :NewEnumerator4 9 :NewEnumerator0 _easy_max_attack_cooldown :NewEnumerator1 _medium_max_attack_cooldown :NewEnumerator2 _hard_max_attack_cooldown :NewEnumerator3 _nightmare_max_attack_cooldown))
    (Components|Sphere|SetSphereRadius (Variables|Default|GetAttack_Radius) (Utilities|Select :Index _difficulty :NewEnumerator4 788.0 :NewEnumerator0 _easy_attack_radius :NewEnumerator1 _medium_attack_radius :NewEnumerator2 _hard_attack_radius :NewEnumerator3 _nightmare_attack_radius) true)
    (Variables|Default|SetAttack%20Delay (Utilities|Select :Index _difficulty :NewEnumerator4 0.5 :NewEnumerator0 _easy_attack_delay :NewEnumerator1 _medium_attack_delay :NewEnumerator2 _hard_attack_delay :NewEnumerator3 _nightmare_attack_delay))
    (else
      (Variables|Default|SetMax_Attack_Cooldown (Utilities|Select :Index (Variables|/Game/SpyroContent/Global_Assets/Global_SaveData/Spyro_Universal_Save_Data.Spyro_Universal_Save_Data_C|GetDifficulty _asspyro_universal_save_data) :NewEnumerator4 9 :NewEnumerator0 _easy_max_attack_cooldown :NewEnumerator1 _medium_max_attack_cooldown :NewEnumerator2 _hard_max_attack_cooldown :NewEnumerator3 _nightmare_max_attack_cooldown))
      (Components|Sphere|SetSphereRadius (Variables|Default|GetAttack_Radius) (Utilities|Select :Index (Variables|/Game/SpyroContent/Global_Assets/Global_SaveData/Spyro_Universal_Save_Data.Spyro_Universal_Save_Data_C|GetDifficulty _asspyro_universal_save_data) :NewEnumerator4 788.0 :NewEnumerator0 _easy_attack_radius :NewEnumerator1 _medium_attack_radius :NewEnumerator2 _hard_attack_radius :NewEnumerator3 _nightmare_attack_radius) true)
      (Variables|Default|SetAttack%20Delay (Utilities|Select :Index (Variables|/Game/SpyroContent/Global_Assets/Global_SaveData/Spyro_Universal_Save_Data.Spyro_Universal_Save_Data_C|GetDifficulty _asspyro_universal_save_data) :NewEnumerator4 0.5 :NewEnumerator0 _easy_attack_delay :NewEnumerator1 _medium_attack_delay :NewEnumerator2 _hard_attack_delay :NewEnumerator3 _nightmare_attack_delay))))
  (if (> (Variables|Default|GetCurrent_Cooldown_Time) (Variables|Default|GetMax_Attack_Cooldown))
    (Variables|Default|SetCurrent_Cooldown_Time (Variables|Default|GetMax_Attack_Cooldown))))

(event EventBeginPlay
  (bind _mesh (Variables|Character|GetMesh))
  (bind _returnvalue (Transformation|GetRelativeTransform _mesh))
  (bind (_location _rotation _scale) (Math|Transform|BreakTransform _returnvalue))
  (|CallParentFunction)
  (Variables|/Game/SpyroContent/Global_Assets/Global_Components/Damageable_Com.Damageable_Com_C|SetComponent_with_Metal_Material (Variables|Default|GetDamageable) (Variables|Character|GetMesh))
  (Variables|Default|SetStartPoint (Transformation|GetActorLocation))
  (bind _output_get (Variables|Default|SetEndPoint (Transformation|GetWorldLocation (Variables|Default|GetMoveTo))))
  (Variables|Default|SetCurrentTarget _output_get)
  (Variables|Default|SetInitial%20Rotation _rotation)
  (Variables|Default|SetInital%20Scale _scale)
  (Variables|Default|SetInitial%20Capsule%20Rotation (.Rotation (Math|Transform|BreakTransform (Transformation|GetRelativeTransform (Variables|Default|GetCapsuleComponent))))))

(fn ConstructionScript
  (|CallParentFunction))