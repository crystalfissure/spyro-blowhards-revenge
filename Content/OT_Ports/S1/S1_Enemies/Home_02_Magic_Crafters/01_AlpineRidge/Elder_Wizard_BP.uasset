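; Elder Wizard enemy Blueprint for Alpine Ridge in the Spyro Magic Crafters homeworld, built on a parent walking AI character.
; It listens for AI state changes and swaps skeletal mesh and animation Blueprint between a normal look when idle and a separate death look when dying.
; Returning to idle also reinitializes the animation Blueprint, and an attack event plays a spatialized sound at the wizard's location.
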(event Custom|Wizard%20State%20Changed
  (bind _mesh (Variables|Character|GetMesh))
  (switch Utilities|FlowControl|Switch|SwitchonAICharacter_States (Variables|/Game/SpyroContent/Global_Assets/Global_Components/Base_AI_Character.Base_AI_Character_C|GetAICharacter_State (Variables|Default|GetWalking_AI_Character))
    (:NewEnumerator0
      (Class|SkinnedMeshComponent|SetSkeletalMesh _mesh (Variables|Default|GetNormal%20Mesh) true)
      (Class|SkeletalMeshComponent|SetAnimClass _mesh (Variables|Default|GetAnim%20BP))
      (CallFunction|ReinitABP))
    (:NewEnumerator3
      (Class|SkinnedMeshComponent|SetSkeletalMesh _mesh (Variables|Default|GetDeath%20Mesh) true)
      (Class|SkeletalMeshComponent|SetAnimClass _mesh "/Game/OT_Ports/S1/S1_Enemies/Home_02_Magic_Crafters/01_AlpineRidge/Elder_Wizard/Elder_Wizard_Death_ABP.Elder_Wizard_Death_ABP_C"))))

(event Custom|Attack%20SFX
  (Audio|PlaySoundatLocation (Variables|Default|GetAttack_SFX) (Transformation|GetActorLocation) "0, 0, 0" 1.0 1.0 0.0 "/Game/SpyroContent/Global_Assets/Global_Audio/Attenuation/Spyro_Attenuation_MediumHigh.Spyro_Attenuation_MediumHigh" 0 0))

(event Custom|Reinit%20ABP
  (bind _aselder_wizard_abp (Utilities|Casting|CastToElder_Wizard_ABP (Components|SkeletalMesh|GetAnimInstance (Variables|Character|GetMesh))))
  (Default|ReinitABP _aselder_wizard_abp))

(event EventBeginPlay
  (|CallParentFunction)
  (EventDispatchers|BindEventtoMyStateChanged (Variables|Default|GetWalking_AI_Character) (delegate Custom|Wizard%20State%20Changed)))

(event Collision|EventActorBeginOverlap
  (params (OtherActor :type Actor%20Object%20Reference))
  (|CallParentFunction OtherActor) ; This node is disabled and will not be called.\nDrag off pins to build functionality.
)

(event EventTick
  (params (DeltaSeconds :type Float%20%28single-precision%29))
  (|CallParentFunction DeltaSeconds) ; This node is disabled and will not be called.\nDrag off pins to build functionality.
)

(fn ConstructionScript
  (|CallParentFunction))