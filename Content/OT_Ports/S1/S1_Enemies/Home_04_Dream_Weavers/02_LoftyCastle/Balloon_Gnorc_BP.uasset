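; Balloon Gnorc enemy for Lofty Castle that floats on a balloon, bobbing around its spawn point via a looping timeline.
; AI state changes are mirrored to the flying AI component and drive gravity, hitbox collision and an Alert-only shield.
; Dying stops the bob, pops the balloon and restores gravity; weapon overlaps run damage checks.
; Shield registration with Damageable stays disconnected because it prevents death from flaming the balloon.
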(event OnComponentBeginOverlap(WeaponHitbox)
  (params (OverlappedComponent :type Primitive%20Component%20Object%20Reference) (OtherActor :type Actor%20Object%20Reference) (OtherComp :type Primitive%20Component%20Object%20Reference) (OtherBodyIndex :type Integer) (bFromSweep :type Boolean) (SweepResult :type Hit%20Result%20Structure%20%28by%20ref%29))
  (CallFunction|DamageCheck OtherActor OtherComp))

(event Custom|On%20State%20Change
  (bind _walking_ai_character (Variables|Default|GetWalking_AI_Character))
  (bind _balloon_mesh (Variables|Default|GetBalloon_Mesh))
  (bind _hitbox (Variables|Default|GetHitbox))
  (bind _shield_hitbox (Variables|Default|GetShield%20Hitbox))
  (bind _charactermovement (Variables|Character|GetCharacterMovement))
  (bind _aicharacter_state (Variables|/Game/SpyroContent/Global_Assets/Global_Components/Base_AI_Character.Base_AI_Character_C|GetAICharacter_State _walking_ai_character))
  (Default|ChangeAICharacterState (Variables|Default|GetFlying_AI_Character) _aicharacter_state)
  (switch Utilities|FlowControl|Switch|SwitchonAICharacter_States _aicharacter_state
    (:NewEnumerator0
      (Variables|/Script/Engine.CharacterMovementComponent|SetGravityScale _charactermovement 0.0 :!label _label))
    (:NewEnumerator1
      (goto _label))
    (:NewEnumerator2
      (goto _label))
    (:NewEnumerator3
      (Variables|/Script/Engine.CharacterMovementComponent|SetGravityScale _charactermovement 1.5)))
  (switch Utilities|FlowControl|Switch|SwitchonAICharacter_States _aicharacter_state
    (:NewEnumerator0
      (Collision|SetCollisionEnabled _shield_hitbox "NoCollision" :!label _label_2))
    (:NewEnumerator1
      (Collision|SetCollisionEnabled _shield_hitbox "QueryAndPhysics"))
    (:NewEnumerator2
      (goto _label_2))
    (:NewEnumerator3
      (goto _label_2)))
  (switch Utilities|FlowControl|Switch|SwitchonAICharacter_States _aicharacter_state
    (:NewEnumerator0
      (Collision|SetCollisionEnabled _hitbox "QueryOnly"))
    (:NewEnumerator3
      (Collision|SetCollisionEnabled _hitbox "NoCollision")))
  (switch Utilities|FlowControl|Switch|SwitchonAICharacter_States _aicharacter_state
    (:NewEnumerator0
      (CallFunction|StartBobbing)
      (Class|SkinnedMeshComponent|SetSkeletalMesh _balloon_mesh "/Game/OT_Ports/S1/S1_Enemies/Home_04_Dream_Weavers/02_LoftyCastle/Balloon_Gnorc/Balloon/Balloon.Balloon" true)
      (Components|Animation|SetAnimation _balloon_mesh "/Game/OT_Ports/S1/S1_Enemies/Home_04_Dream_Weavers/02_LoftyCastle/Balloon_Gnorc/Balloon/Balloon_Anim.Balloon_Anim")
      (Transformation|SetRelativeScale3D _balloon_mesh "-0.250000,0.250000,0.250000"))
    (:NewEnumerator3
      (CallFunction|StopBobbing)
      (Class|SkinnedMeshComponent|SetSkeletalMesh _balloon_mesh "/Game/OT_Ports/S1/S1_Enemies/Home_04_Dream_Weavers/02_LoftyCastle/Balloon_Gnorc/Balloon/Balloon_Pop.Balloon_Pop" true)
      (Components|Animation|SetAnimation _balloon_mesh "/Game/OT_Ports/S1/S1_Enemies/Home_04_Dream_Weavers/02_LoftyCastle/Balloon_Gnorc/Balloon/Balloon_Pop_Anim.Balloon_Pop_Anim")
      (Transformation|SetRelativeScale3D _balloon_mesh "-0.500000,0.500000,0.500000"))))

(event Custom|Character%20melted
  (Components|Movement|StopMovementImmediately (Variables|Character|GetCharacterMovement)))

(event Custom|Start%20Bobbing
  (bind _newtrack_0 (Timeline|Bobbing PlayFromStart)
    (:Update
      (Transformation|SetActorRelativeLocation (Math|Vector|MakeVector (Variables|Default|GetInitial%20Location%20X) (Variables|Default|GetInitial%20Location%20Y) (+ (Variables|Default|GetInitial%20Location%20Z) (* _newtrack_0 4.0)))))
    (:Finished
      (CallFunction|StartBobbing))))

(event Custom|Stop%20Bobbing
  (bind _newtrack_0 (Timeline|Bobbing Stop)
    (:Update
      (Transformation|SetActorRelativeLocation (Math|Vector|MakeVector (Variables|Default|GetInitial%20Location%20X) (Variables|Default|GetInitial%20Location%20Y) (+ (Variables|Default|GetInitial%20Location%20Z) (* _newtrack_0 4.0)))))
    (:Finished
      (CallFunction|StartBobbing))))

(event EventBeginPlay
  (bind _returnvalue (Transformation|GetActorLocation))
  (|CallParentFunction)
  (EventDispatchers|BindEventtoMyStateChanged (Variables|Default|GetWalking_AI_Character) (delegate Custom|On%20State%20Change))
  (Variables|/Game/SpyroContent/Global_Assets/Global_Components/Damageable_Com.Damageable_Com_C|SetComponent_with_Metal_Material (Variables|Default|GetDamageable) (Variables|Character|GetMesh))
  (EventDispatchers|BindEventtoMeltedfromIce (Variables|Default|GetDamageable) (delegate Custom|Character%20melted))
  (EventDispatchers|BindEventtoCallStopBeingAfraid (Variables|Default|GetDamageable) (delegate Custom|Character%20melted))
  (Variables|/Game/SpyroContent/Global_Assets/Global_Components/Damageable_Com.Damageable_Com_C|SetObject's%20Hitbox%20Component (Variables|Default|GetDamageable) (Variables|Default|GetHitbox))
  (Variables|Default|SetInitial%20Location%20X (.x _returnvalue))
  (Variables|Default|SetInitial%20Location%20Y (.y _returnvalue))
  (Variables|Default|SetInitial%20Location%20Z (.z _returnvalue))
  (CallFunction|StartBobbing)
  (Components|Timeline|SetPlayRate (Variables|Default|GetBobbing) (Variables|Default|GetBobbing%20Cycle%20Rate)))

(event Collision|EventActorBeginOverlap
  (params (OtherActor :type Actor%20Object%20Reference)))

(event EventTick
  (params (DeltaSeconds :type Float%20%28single-precision%29))
  (|CallParentFunction DeltaSeconds) ; This node is disabled and will not be called.\nDrag off pins to build functionality.
)

(fn ConstructionScript
  (|CallParentFunction))