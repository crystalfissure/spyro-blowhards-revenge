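; Chicken fodder Blueprint for the Beast Makers home in the Spyro S1 content, adding periodic idle sounds to its parent's behavior.
; BeginPlay starts an endless loop that waits a random few seconds, then calls ChickenIdleSFX, which wires back into the same Delay.
; Each pass plays the chicken sound at the actor's location with Spyro attenuation, unless the WalkingAICharacter's state matches one specific enum value.
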(event Custom|Chicken%20Idle%20SFX
  (if (Utilities|Enum|Equal(Enum) (Variables|/Game/SpyroContent/Global_Assets/Global_Components/Base_AI_Character.Base_AI_Character_C|GetAICharacter_State (Variables|Default|GetWalking_AI_Character)) "NewEnumerator3")
    _
    (else
      (Audio|PlaySoundatLocation "/Game/OT_Ports/S1/S1_Fodder/Home_03_Beast_Makers/Chicken/Chicken_SFX.Chicken_SFX" (Transformation|GetActorLocation) "0, 0, 0" 1.0 1.0 0.0 "/Game/SpyroContent/Global_Assets/Global_Audio/Attenuation/Spyro_Attenuation.Spyro_Attenuation" 0 0)))
  (Utilities|FlowControl|Delay (Math|Random|RandomFloatinRange 2.0 3.0))
  (CallFunction|ChickenIdleSFX))

(event EventBeginPlay
  (|CallParentFunction)
  (Utilities|FlowControl|Delay (Math|Random|RandomFloatinRange 2.0 3.0))
  (CallFunction|ChickenIdleSFX))

(event Collision|EventActorBeginOverlap
  (params (OtherActor :type Actor%20Object%20Reference)))

(event EventTick
  (params (DeltaSeconds :type Float%20%28single-precision%29)))

(fn ConstructionScript
  (|CallParentFunction))