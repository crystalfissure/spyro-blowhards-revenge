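; Dragon egg collectible for the S1 port that spins continuously through a self-restarting timeline.
; Overlapping the player capsule, or the NPCAwardItem component's award-spawned event, saves it to Spyro_PersistantData, plays burst and sound effects, and destroys it.
; When NPCAwardItem reports its thief died, a second timeline lerps the egg toward the player.
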(event OnComponentBeginOverlap(Hitbox)
  (params (OverlappedComponent :type Primitive%20Component%20Object%20Reference) (OtherActor :type Actor%20Object%20Reference) (OtherComp :type Primitive%20Component%20Object%20Reference) (OtherBodyIndex :type Integer) (bFromSweep :type Boolean) (SweepResult :type Hit%20Result%20Structure%20%28by%20ref%29))
  (bind _returnvalue (Transformation|GetActorLocation))
  (bind (_x _y _z) (Math|Vector|BreakVector _returnvalue))
  (bind _returnvalue_2 (- _z 5e+01))
  (bind _returnvalue_3 (Math|Vector|MakeVector _x _y _returnvalue_2))
  (bind _asbp_base_playable (Utilities|Casting|CastToBP_Base_Playable OtherActor))
  (if (== (Variables|/Script/Engine.Character|GetCapsuleComponent _asbp_base_playable) OtherComp)
    (bind _asspyro_persistant_data (Utilities|Casting|CastToSpyro_PersistantData (Game|GetGameInstance)))
    (Default|SaveACollectible _asspyro_persistant_data "NewEnumerator4" "" 0.0 (Variables|/Game/SpyroContent/Global_Assets/Global_Components/NPC_Award_Item.NPC_Award_Item_C|GetLevel%20Item%20Index (Variables|Default|GetNPC_Award_Item)) 5.0)
    (Effects|SpawnEmitteratLocation "/Game/OT_Ports/S1/S1_LevelItems/Dragon_Egg_S1/Assets/Dragon_Egg_S1_Burst.Dragon_Egg_S1_Burst" _returnvalue_3)
    (Audio|PlaySoundatLocation "/Game/SpyroContent/Global_Assets/Global_Level_Items/Butterflies/Audio/1UP.1UP" _returnvalue_3 "0, 0, 0" 1.0 1.0 0.0 0 0 0)
    (Actor|DestroyActor)))

(event Custom|Manage%20Rotation
  (bind _newtrack_0 (Timeline|Timeline_0 PlayFromStart)
    (:Update
      (Transformation|SetRelativeRotation (Variables|Default|GetDragon_Egg_S1) (Math|Rotator|MakeRotator 0.0 0.0 _newtrack_0) false false))
    (:Finished
      (CallFunction|ManageRotation))))

(event Custom|NPC%20Reward%20Process
  (bind _returnvalue (Transformation|GetActorLocation))
  (bind (_x _y _z) (Math|Vector|BreakVector _returnvalue))
  (bind _returnvalue_2 (- _z 5e+01))
  (bind _returnvalue_3 (Math|Vector|MakeVector _x _y _returnvalue_2))
  (bind _asspyro_persistant_data (Utilities|Casting|CastToSpyro_PersistantData (Game|GetGameInstance)))
  (Default|SaveACollectible _asspyro_persistant_data "NewEnumerator4" "" 0.0 (Variables|/Game/SpyroContent/Global_Assets/Global_Components/NPC_Award_Item.NPC_Award_Item_C|GetLevel%20Item%20Index (Variables|Default|GetNPC_Award_Item)) 5.0)
  (Effects|SpawnEmitteratLocation "/Game/OT_Ports/S1/S1_LevelItems/Dragon_Egg_S1/Assets/Dragon_Egg_S1_Burst.Dragon_Egg_S1_Burst" _returnvalue_3)
  (Audio|PlaySoundatLocation "/Game/SpyroContent/Global_Assets/Global_Level_Items/Butterflies/Audio/1UP.1UP" _returnvalue_3 "0, 0, 0" 1.0 1.0 0.0 0 0 0)
  (Actor|DestroyActor))

(event Custom|Home%20to%20Spyro
  (bind _newtrack_0 (Timeline|Timeline_1 PlayFromStart)
    (:Update
      (bind _returnvalue (Actor|GetActorOfClass "/Game/SpyroContent/Global_Assets/Global_Characters/Playable_Characters/BP_Base_Playable.BP_Base_Playable_C"))
      (Transformation|SetActorLocation (Math|Vector|Lerp(Vector) (Transformation|GetActorLocation) (Transformation|GetActorLocation _returnvalue) _newtrack_0) false false))))

(event EventBeginPlay
  (bind _npc_award_item (Variables|Default|GetNPC_Award_Item))
  (CallFunction|ManageRotation)
  (EventDispatchers|BindEventtoNPCAwardSpawned _npc_award_item (delegate Custom|NPC%20Reward%20Process))
  (EventDispatchers|BindEventtoMyThiefDied _npc_award_item (delegate Custom|Home%20to%20Spyro)))

(fn ConstructionScript)