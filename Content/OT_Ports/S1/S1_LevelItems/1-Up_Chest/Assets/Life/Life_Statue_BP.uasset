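; Spyro life statue pickup that spins on a looping timeline and grants an extra life when the player's capsule first overlaps it.
; Collection polls until the item has a unique name and valid level index, then calls GainALife on the player controller.
; It then saves the collectible to persistent game-instance data, updates skill level, plays burst and sound effects, and destroys itself.
; Thief-stealing logic is present but disconnected.
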(event OnComponentBeginOverlap(Hitbox)
  (params (OverlappedComponent :type Primitive%20Component%20Object%20Reference) (OtherActor :type Actor%20Object%20Reference) (OtherComp :type Primitive%20Component%20Object%20Reference) (OtherBodyIndex :type Integer) (bFromSweep :type Boolean) (SweepResult :type Hit%20Result%20Structure%20%28by%20ref%29))
  (bind _emitter_spawn_location (Variables|Default|GetEmitter%20Spawn%20Location))
  (bind _returnvalue (Transformation|GetWorldLocation _emitter_spawn_location))
  (bind _asbp_base_playable (Utilities|Casting|CastToBP_Base_Playable OtherActor))
  (if (== (Variables|/Script/Engine.Character|GetCapsuleComponent _asbp_base_playable) OtherComp)
    (Utilities|FlowControl|DoOnce false
      (:Completed
        (if (or (Utilities|Enum|Equal(Enum) (Variables|Default|GetMy_Unique_Name) "DEFAULT") (< (Variables|Default|GetLevel%20Item%20Index) 0))
          (Utilities|FlowControl|Delay 0.2)
          (CallFunction|DoIHaveANameYet?)
          (else
            (bind _asspyro_player_controller (Utilities|Casting|CastToSpyro_PlayerController (Pawn|GetController _asbp_base_playable))
              (:then
                (Default|GainALife _asspyro_player_controller (Variables|Default|GetLevel%20Item%20Index)))
              (:CastFailed
                _))
            (Utilities|FlowControl|Delay 0.2)
            (if (Utilities|Enum|Equal(Enum) (Variables|Default|GetMy_Unique_Name) "DEFAULT")
              (Development|PrintString "FAILED TO SAVE BLUE BUTTERFLY DUE TO LACKING A UNIQUE NAME. WAS IT SPAWNED IN PROPERLY?")
              (else
                (bind _asspyro_persistant_data (Utilities|Casting|CastToSpyro_PersistantData (Game|GetGameInstance)))
                (Default|SaveACollectible _asspyro_persistant_data "NewEnumerator2" (Variables|Default|GetMy_Unique_Name) 0.0 (Variables|Default|GetLevel%20Item%20Index) 0.0)
                (Default|CallSavedACollectable)
                (CallFunction|UpdateSkillLevel (Variables|Default|GetSkill%20Level%20Award) self)
                (Effects|SpawnEmitteratLocation "/Game/SpyroContent/Global_Assets/Global_Level_Items/Dragon_Breath/Particles/flame_burst_particle_1.flame_burst_particle_1" _returnvalue)
                (Audio|PlaySoundatLocation "/Game/SpyroContent/Global_Assets/Global_Level_Items/Butterflies/Audio/1UP.1UP" _returnvalue "0, 0, 0" 1.0 1.0 0.0 0 0 0)
                (Actor|DestroyActor)))))))))

(event Custom|Manage%20Rotation
  (bind _newtrack_0 (Timeline|Timeline_0 PlayFromStart)
    (:Update
      (Transformation|SetRelativeRotation (Variables|Default|GetStaticMesh) (Math|Rotator|MakeRotator 0.0 0.0 _newtrack_0) false false))
    (:Finished
      (CallFunction|ManageRotation))))

(event Custom|do%20i%20have%20a%20name%20yet?
  (bind _emitter_spawn_location (Variables|Default|GetEmitter%20Spawn%20Location))
  (bind _returnvalue (Transformation|GetWorldLocation _emitter_spawn_location))
  (if (or (Utilities|Enum|Equal(Enum) (Variables|Default|GetMy_Unique_Name) "DEFAULT") (< (Variables|Default|GetLevel%20Item%20Index) 0))
    (Utilities|FlowControl|Delay 0.2)
    (CallFunction|DoIHaveANameYet?)
    (else
      (bind _asspyro_player_controller (Utilities|Casting|CastToSpyro_PlayerController (Pawn|GetController (stale OnComponentBeginOverlap(Hitbox) _asbp_base_playable)))
        (:then
          (Default|GainALife _asspyro_player_controller (Variables|Default|GetLevel%20Item%20Index)))
        (:CastFailed
          _))
      (Utilities|FlowControl|Delay 0.2)
      (if (Utilities|Enum|Equal(Enum) (Variables|Default|GetMy_Unique_Name) "DEFAULT")
        (Development|PrintString "FAILED TO SAVE BLUE BUTTERFLY DUE TO LACKING A UNIQUE NAME. WAS IT SPAWNED IN PROPERLY?")
        (else
          (bind _asspyro_persistant_data (Utilities|Casting|CastToSpyro_PersistantData (Game|GetGameInstance)))
          (Default|SaveACollectible _asspyro_persistant_data "NewEnumerator2" (Variables|Default|GetMy_Unique_Name) 0.0 (Variables|Default|GetLevel%20Item%20Index) 0.0)
          (Default|CallSavedACollectable)
          (CallFunction|UpdateSkillLevel (Variables|Default|GetSkill%20Level%20Award) self)
          (Effects|SpawnEmitteratLocation "/Game/SpyroContent/Global_Assets/Global_Level_Items/Dragon_Breath/Particles/flame_burst_particle_1.flame_burst_particle_1" _returnvalue)
          (Audio|PlaySoundatLocation "/Game/SpyroContent/Global_Assets/Global_Level_Items/Butterflies/Audio/1UP.1UP" _returnvalue "0, 0, 0" 1.0 1.0 0.0 0 0 0)
          (Actor|DestroyActor))))))

(event Custom|Stolen%20By%20Thief
  (Variables|Default|SetStolen%20by%20a%20thief true))

(event EventBeginPlay
  (CallFunction|ManageRotation))

(fn ConstructionScript)