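; Statue burst actor for the Dragon Statue level item that triggers a shard effect, then removes itself.
; ShardBurstAction loops over two child actor components, casts each to Basket_Shard_BP and passes both shard meshes to its ShardAction.
; After a short delay the actor destroys itself.
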(event EventBeginPlay)

(event Collision|EventActorBeginOverlap
  (params (OtherActor :type Actor%20Object%20Reference)))

(event EventTick
  (params (DeltaSeconds :type Float%20%28single-precision%29)))

(event EventShardBurstAction
  (params (Shard%20Mesh%201 :type Static%20Mesh%20Object%20Reference) (Shard%20Mesh%202 :type Static%20Mesh%20Object%20Reference))
  (for _array_element (Utilities|Array|MakeArray (Variables|Default|GetChildActor) (Variables|Default|GetChildActor1))
    (bind _asbasket_shard_bp (Utilities|Casting|CastToBasket_Shard_BP (Variables|/Script/Engine.ChildActorComponent|GetChildActor _array_element)))
    (Default|ShardAction _asbasket_shard_bp Shard%20Mesh%201 Shard%20Mesh%202))
  (Utilities|FlowControl|Delay 2.1)
  (Actor|DestroyActor))

(fn ConstructionScript
  (|CallParentFunction))