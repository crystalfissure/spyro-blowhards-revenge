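; Spawner actor that spits out a super-damage spittable rock when its SpawnLavaRock event runs, using the GreenRock flag to pick the lava or green variant.
; The rock spawns at a forward offset, gets its spittable state set, and is launched with physics by an up-and-forward velocity-change impulse.
; It stores a reference back to this spawner, and a spit sound plays at the spawner's location.
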(event EventBeginPlay
  (|CallParentFunction) ; This node is disabled and will not be called.\nDrag off pins to build functionality.
)

(event Collision|EventActorBeginOverlap
  (params (OtherActor :type Actor%20Object%20Reference)))

(event EventTick
  (params (DeltaSeconds :type Float%20%28single-precision%29)))

(event EventSpawnLavaRock
  (bind _returnvalue (Transformation|GetActorForwardVector))
  (bind _returnvalue_2 (Transformation|GetActorLocation))
  (bind _returnvalue_3 (Transformation|GetActorTransform))
  (bind _returnvalue_4 (Transformation|GetActorUpVector))
  (bind _returnvalue_5 (Transformation|GetActorForwardVector))
  (bind _self self)
  (bind _forward_offset (Variables|Default|Getforward%20offset))
  (bind _returnvalue_6 (* _returnvalue _forward_offset))
  (bind _returnvalue_7 (* _returnvalue_4 5e+02))
  (bind _returnvalue_8 (* _returnvalue_5 2.5e+02))
  (bind _returnvalue_9 (+ _returnvalue_7 _returnvalue_8))
  (bind _returnvalue_10 (+ (.location _returnvalue_3) _returnvalue_6))
  (if (not (Variables|Default|GetGreen%20Rock))
    (bind _returnvalue_11 (Game|SpawnActorfromClass "/Game/OT_Ports/Global/Level_Items/Spittable/LavaRock_SuperDamage_BP.LavaRock_SuperDamage_BP_C" (Math|Transform|MakeTransform _returnvalue_10 "0, 0, 0" "1,1,1") "AdjustIfPossibleButAlwaysSpawn" 0 0))
    (Variables|/Game/SpyroContent/Global_Assets/Global_Level_Items/Spittable_Object/Base_Spittable_Object_BP.Base_Spittable_Object_BP_C|SetSpittable%20Object%20State _returnvalue_11 "NewEnumerator1")
    (Physics|SetSimulatePhysics (Variables|/Game/SpyroContent/Global_Assets/Global_Level_Items/Spittable_Object/Base_Spittable_Object_BP.Base_Spittable_Object_BP_C|GetCOL _returnvalue_11) true)
    (Physics|AddImpulse (Variables|/Game/SpyroContent/Global_Assets/Global_Level_Items/Spittable_Object/Base_Spittable_Object_BP.Base_Spittable_Object_BP_C|GetCOL _returnvalue_11) _returnvalue_9 "None" true)
    (Variables|/Game/SpyroContent/Global_Assets/Global_Level_Items/Spittable_Object/LavaRock/LavaRock_BP.LavaRock_BP_C|SetMy%20Spawner _returnvalue_11 _self)
    (Audio|PlaySoundatLocation "/Game/SpyroContent/Global_Assets/Global_Level_Items/Spittable_Object/LavaRock/lava_rock_spit.lava_rock_spit" _returnvalue_2 "0, 0, 0" 1.0 1.0 0.0 "/Game/SpyroContent/Global_Assets/Global_Audio/Attenuation/Spyro_Attenuation_MediumHigh.Spyro_Attenuation_MediumHigh" 0 0)
    (else
      (bind _returnvalue_12 (Game|SpawnActorfromClass "/Game/OT_Ports/Global/Level_Items/Spittable/GreenRock_SuperDamage_BP.GreenRock_SuperDamage_BP_C" (Math|Transform|MakeTransform _returnvalue_10 "0, 0, 0" "1,1,1") "AdjustIfPossibleButAlwaysSpawn" 0 0))
      (Variables|/Game/SpyroContent/Global_Assets/Global_Level_Items/Spittable_Object/Base_Spittable_Object_BP.Base_Spittable_Object_BP_C|SetSpittable%20Object%20State _returnvalue_12 "NewEnumerator1")
      (Physics|SetSimulatePhysics (Variables|/Game/SpyroContent/Global_Assets/Global_Level_Items/Spittable_Object/Base_Spittable_Object_BP.Base_Spittable_Object_BP_C|GetCOL _returnvalue_12) true)
      (Physics|AddImpulse (Variables|/Game/SpyroContent/Global_Assets/Global_Level_Items/Spittable_Object/Base_Spittable_Object_BP.Base_Spittable_Object_BP_C|GetCOL _returnvalue_12) _returnvalue_9 "None" true)
      (Variables|/Game/SpyroContent/Global_Assets/Global_Level_Items/Spittable_Object/LavaRock/LavaRock_BP.LavaRock_BP_C|SetMy%20Spawner _returnvalue_12 _self)
      (Audio|PlaySoundatLocation "/Game/SpyroContent/Global_Assets/Global_Level_Items/Spittable_Object/LavaRock/lava_rock_spit.lava_rock_spit" _returnvalue_2 "0, 0, 0" 1.0 1.0 0.0 "/Game/SpyroContent/Global_Assets/Global_Audio/Attenuation/Spyro_Attenuation_MediumHigh.Spyro_Attenuation_MediumHigh" 0 0))))

(fn ConstructionScript
  (|CallParentFunction))