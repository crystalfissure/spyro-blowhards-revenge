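; LavaRock_SuperDamage_BP is a spittable lava rock that deals super damage to what it hits, then destroys itself.
; It replaces the parent's Damage Target logic, skipping walking AI characters in one particular state and already-destroyed treasure containers.
; Hits pass the rock's forward vector and credit the player who last spat it, when that player is valid.
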(event EventBeginPlay
  (|CallParentFunction) ; This node is disabled and will not be called.\nDrag off pins to build functionality.
)

(event Collision|EventActorBeginOverlap
  (params (OtherActor :type Actor%20Object%20Reference)))

(event EventTick
  (params (DeltaSeconds :type Float%20%28single-precision%29))
  (|CallParentFunction DeltaSeconds) ; This node is disabled and will not be called.\nDrag off pins to build functionality.
)

(fn ConstructionScript
  (|CallParentFunction))

(fn DamageTarget
  (params (damag%20comp :type Damageable%20Com%20Object%20Reference))
  (bind _returnvalue (Components|GetOwner damag%20comp))
  (bind _returnvalue_2 (Transformation|GetActorForwardVector))
  (bind _returnvalue_3 (Actor|GetComponentbyClass _returnvalue "/Game/SpyroContent/Global_Assets/Global_Components/Child_Components/Walking_AI_Character.Walking_AI_Character_C"))
  (Utilities|IsValid _returnvalue_3
    (:Is%20Valid
      (if (not (Utilities|Enum|Equal(Enum) (Variables|/Game/SpyroContent/Global_Assets/Global_Components/Base_AI_Character.Base_AI_Character_C|GetAICharacter_State _returnvalue_3) "NewEnumerator3"))
        (bind _player_who_last_spat_me (Variables|Default|GetPlayer%20Who%20Last%20Spat%20Me :!label _label)
          (:then
            (Default|DealDamage damag%20comp "NewEnumerator4" _returnvalue_2 true _player_who_last_spat_me false))
          (:else
            (Default|DealDamage damag%20comp "NewEnumerator4" _returnvalue_2 true 0 false)))
        (Development|PrintString "rock destroyed by damage target")
        (Actor|DestroyActor)))
    (:Is%20Not%20Valid
      (bind _astreasure_container_base_bp (Utilities|Casting|CastToTreasure_Container_Base_BP _returnvalue)
        (:then
          (if (not (Variables|/Game/SpyroContent/Global_Assets/Global_Level_Items/Treasure_Containers/Treasure_Container_Base_BP.Treasure_Container_Base_BP_C|GetContainer_Destroyed _astreasure_container_base_bp))
            (goto _label)))
        (:CastFailed
          (goto _label))))))