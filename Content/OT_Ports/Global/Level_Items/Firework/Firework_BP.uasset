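; Firework actor that, when hit by one specific damage type, launches along a spline to blast its assigned target.
; After a delay, Tick moves and orients the mesh along the spline.
; At the spline's end it applies super damage directly to MyTarget, hides itself and plays blast effects.
; Container or enemy item-drop resets rearm it at the spline start; destroying a container target also destroys it.
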(event CallDealDamage(Damageable_Com)
  (if (not (Variables|Default|GetisDetonated))
    (if (Utilities|Enum|Equal(Enum) (Variables|/Game/SpyroContent/Global_Assets/Global_Components/Damageable_Com.Damageable_Com_C|GetDeal%20Damage%20-%20Damage%20Type (Variables|Default|GetDamageable_Com)) "NewEnumerator1")
      (Utilities|FlowControl|DoOnce false
        (:Completed
          (CallFunction|SetOffFirework))))))

(event DamageWasAttempted(Damageable_Com))

(event Custom|Set%20Off%20Firework
  (Components|Activation|Activate (Variables|Default|GetParticleSystem) false)
  (Utilities|FlowControl|Delay (Variables|Default|GetDelay))
  (Variables|Default|SetisFlying true))

(event Custom|Detonate%20Firework
  (bind _staticmesh (Variables|Default|GetStaticMesh))
  (bind _returnvalue (Transformation|GetWorldLocation _staticmesh))
  (Default|DealDamage (Actor|GetComponentbyClass (Variables|Default|GetMy%20Target) "/Game/SpyroContent/Global_Assets/Global_Components/Damageable_Com.Damageable_Com_C") "NewEnumerator4" (Math|Vector|GetForwardVector (Variables|Default|GetStaticMesh)) true 0 false)
  (Components|Activation|Deactivate (Variables|Default|GetParticleSystem))
  (Rendering|SetVisibility (Variables|Default|GetStaticMesh) false false)
  (Variables|Default|SetisDetonated true)
  (Effects|SpawnEmitteratLocation "/Game/SpyroContent/Global_Assets/Global_Level_Items/Superflame/Particles/Superflame_Blast.Superflame_Blast" _returnvalue)
  (Audio|PlaySoundatLocation "/Game/SpyroContent/Global_Assets/Global_Level_Items/Superflame/Audio/superflame_impact.superflame_impact" _returnvalue "0, 0, 0" 1.0 1.0 0.0 "/Game/SpyroContent/Global_Assets/Global_Audio/Attenuation/Spyro_Attenuation_Even_Farther.Spyro_Attenuation_Even_Farther" 0 0))

(event Custom|Reset%20Firework
  (Variables|Default|SetCurrentSplineDistance 0.0)
  (Variables|Default|SetisFlying false)
  (Components|Activation|Deactivate (Variables|Default|GetParticleSystem))
  (Rendering|SetVisibility (Variables|Default|GetStaticMesh) true false)
  (Variables|Default|SetisDetonated false)
  (CallFunction|SetOffFireworkReset)
  (CallFunction|ResetFireworkLocation))

(event Custom|Set%20Off%20Firework%20Reset
  (Utilities|FlowControl|DoOnce false) ; enters at Reset
)

(event Custom|Reset%20Firework%20-%20Container%20Reset
  (CallFunction|ResetFirework))

(event Custom|Reset%20Firework%20-%20Enemy%20Reset
  (CallFunction|ResetFirework))

(event Custom|Reset%20Firework%20Location
  (bind _spline (Variables|Default|GetSpline))
  (bind _currentsplinedistance (Variables|Default|GetCurrentSplineDistance))
  (bind _spline_2 (Variables|Default|GetSpline))
  (bind _currentsplinedistance_2 (Variables|Default|GetCurrentSplineDistance))
  (bind _returnvalue (Spline|GetLocationatDistanceAlongSpline _spline_2 _currentsplinedistance "World"))
  (bind _returnvalue_2 (+ _currentsplinedistance_2 5e+01))
  (bind _returnvalue_3 (Spline|GetLocationatDistanceAlongSpline _spline _returnvalue_2 "World"))
  (bind _returnvalue_4 (Math|Rotator|FindLookatRotation _returnvalue _returnvalue_3))
  (Transformation|SetWorldLocation (Variables|Default|GetStaticMesh) _returnvalue false false)
  (Transformation|SetWorldRotation (Variables|Default|GetStaticMesh) (Math|Rotator|MakeRotator 0.0 (+ (.pitch _returnvalue_4) -9e+01) (.yaw _returnvalue_4)) false false))

(event Custom|Destroy%20Actor
  (params (DestroyedActor :type Actor%20Object%20Reference))
  (Actor|DestroyActor))

(event EventBeginPlay
  (bind _my_target (Variables|Default|GetMy%20Target))
  (Variables|/Game/SpyroContent/Global_Assets/Global_Components/Damageable_Com.Damageable_Com_C|SetObject's%20Hitbox%20Component (Variables|Default|GetDamageable_Com) (Variables|Default|GetBox))
  (Utilities|IsValid (Actor|GetComponentbyClass (Variables|Default|GetMy%20Target) "/Game/SpyroContent/Global_Assets/Global_Components/Damageable_Com.Damageable_Com_C")
    (:Is%20Valid
      (Utilities|FlowControl|Sequence
        (:then_0
          (bind _astreasure_container_base_bp (Utilities|Casting|CastToTreasure_Container_Base_BP _my_target))
          (EventDispatchers|BindEventtoItemDropperSuccessfullyReset (Variables|/Game/SpyroContent/Global_Assets/Global_Level_Items/Treasure_Containers/Treasure_Container_Base_BP.Treasure_Container_Base_BP_C|GetItem_Drop_Component _astreasure_container_base_bp) (delegate Custom|Reset%20Firework%20-%20Container%20Reset))
          (Game|BindEventtoOnDestroyed _astreasure_container_base_bp (delegate Custom|Destroy%20Actor)))
        (:then_1
          (bind _asbase_enemy_bp (Utilities|Casting|CastToBase_Enemy_BP _my_target))
          (EventDispatchers|BindEventtoItemDropperSuccessfullyReset (Variables|/Game/SpyroContent/Global_Assets/Global_Characters/AI_Characters/Actors/Base_AICharacter_BP.Base_AICharacter_BP_C|GetDrops_Items _asbase_enemy_bp) (delegate Custom|Reset%20Firework%20-%20Enemy%20Reset)))))
    (:Is%20Not%20Valid
      (Development|PrintString "Firework_BP:::My Target doesn't have Damageable component!"))))

(event EventTick
  (params (DeltaSeconds :type Float%20%28single-precision%29))
  (if (Variables|Default|GetisFlying)
    (Variables|Default|SetCurrentSplineDistance (+ (Variables|Default|GetCurrentSplineDistance) (* (Variables|Default|GetFlying%20Speed) DeltaSeconds)))
    (if (>= (+ (Variables|Default|GetCurrentSplineDistance) (* (Variables|Default|GetFlying%20Speed) DeltaSeconds)) (Spline|GetSplineLength (Variables|Default|GetSpline)))
      (Variables|Default|SetisFlying false)
      (CallFunction|DetonateFirework)
      (else
        (Transformation|SetWorldLocation (Variables|Default|GetStaticMesh) (Spline|GetLocationatDistanceAlongSpline (Variables|Default|GetSpline) (Variables|Default|GetCurrentSplineDistance) "World") false false)
        (Transformation|SetWorldRotation (Variables|Default|GetStaticMesh) (Math|Rotator|MakeRotator 0.0 (+ (.pitch (Math|Rotator|FindLookatRotation (Spline|GetLocationatDistanceAlongSpline (Variables|Default|GetSpline) (Variables|Default|GetCurrentSplineDistance) "World") (Spline|GetLocationatDistanceAlongSpline (Variables|Default|GetSpline) (+ (Variables|Default|GetCurrentSplineDistance) 5e+01) "World"))) -9e+01) (.yaw (Math|Rotator|FindLookatRotation (Spline|GetLocationatDistanceAlongSpline (Variables|Default|GetSpline) (Variables|Default|GetCurrentSplineDistance) "World") (Spline|GetLocationatDistanceAlongSpline (Variables|Default|GetSpline) (+ (Variables|Default|GetCurrentSplineDistance) 5e+01) "World")))) false false)))))

(fn ConstructionScript)