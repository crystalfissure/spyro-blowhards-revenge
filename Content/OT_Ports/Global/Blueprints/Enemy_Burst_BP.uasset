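; Enemy burst effect actor that drives shard child actors and then removes itself.
; ShardBurstAction passes a shard mesh to the Enemy_Shard_BP child's ShardAction, then destroys the burst after a short delay.
; A separate Activate Black Smoke function casts child actors to Basket_Shard_BP, a different class from the burst event, and activates their smoke component.
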(event Custom|Shard%20Burst%20Action
  (params (Shard%20Mesh%201 :type Static%20Mesh%20Object%20Reference))
  (for _array_element (Utilities|Array|MakeArray (Variables|Default|GetChildActor))
    (bind _asenemy_shard_bp (Utilities|Casting|CastToEnemy_Shard_BP (Variables|/Script/Engine.ChildActorComponent|GetChildActor _array_element)))
    (Default|ShardAction _asenemy_shard_bp Shard%20Mesh%201))
  (Utilities|FlowControl|Delay 2.1)
  (Actor|DestroyActor))

(fn ConstructionScript)

(fn ActivateBlackSmoke
  (for _array_element (Utilities|Array|MakeArray (Variables|Default|GetChildActor) 0 0 0 0 0 0 0 0 0)
    (bind _asbasket_shard_bp (Utilities|Casting|CastToBasket_Shard_BP (Variables|/Script/Engine.ChildActorComponent|GetChildActor _array_element)))
    (Components|Activation|Activate (Variables|/Game/SpyroContent/Global_Assets/Global_Level_Items/Treasure_Containers/Basket/Actors/Basket_Shard_BP.Basket_Shard_BP_C|Getbasket_shard_smoke _asbasket_shard_bp) false)))