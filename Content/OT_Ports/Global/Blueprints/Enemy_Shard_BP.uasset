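; Debris actor for an enemy shard that flies out, optionally pops and cleans itself up.
; ShardAction assigns the supplied mesh, randomly jitters its position and yaw, then launches it forward and upward with a velocity-change impulse.
; After a short random delay it hides the mesh, randomly firing PopParticle first, then destroys the actor a few seconds later.
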(event Custom|Shard%20Action
  (params (Shard%20Mesh%201 :type Static%20Mesh%20Object%20Reference))
  (bind _returnvalue (Math|Random|RandomFloatinRange -1e+01 1e+01))
  (bind _returnvalue_2 (Math|Random|RandomFloatinRange 175.0 275.0))
  (bind _staticmesh (Variables|Default|GetStaticMesh))
  (bind _staticmesh_2 (Variables|Default|GetStaticMesh))
  (bind _returnvalue_3 (Transformation|GetWorldLocation _staticmesh_2))
  (bind _returnvalue_4 (Math|Vector|GetForwardVector _staticmesh))
  (bind _returnvalue_5 (Transformation|GetWorldRotation _staticmesh_2))
  (bind _returnvalue_6 (* _returnvalue_4 _returnvalue_2))
  (Components|StaticMesh|SetStaticMesh (Variables|Default|GetStaticMesh) Shard%20Mesh%201)
  (Transformation|SetWorldLocationAndRotation _staticmesh_2 (Math|Vector|MakeVector (+ (.x _returnvalue_3) _returnvalue) (+ (.y _returnvalue_3) _returnvalue) (+ (.z _returnvalue_3) _returnvalue)) (Math|Rotator|MakeRotator (.roll _returnvalue_5) (.pitch _returnvalue_5) (+ (.yaw _returnvalue_5) _returnvalue)) false false)
  (Physics|AddImpulse _staticmesh (Math|Vector|MakeVector (.x _returnvalue_6) (.y _returnvalue_6) (+ (.z _returnvalue_6) 3.5e+02)) "None" true)
  (Utilities|FlowControl|Delay (Math|Random|RandomFloatinRange 0.5 1.73))
  (if (Math|Random|RandomBool)
    (Components|Activation|Activate (Variables|Default|Getpop_particle) false))
  (Rendering|SetVisibility (Variables|Default|GetStaticMesh) false false)
  (Utilities|FlowControl|Delay 5.0)
  (Actor|DestroyActor))

(event EventTick
  (params (DeltaSeconds :type Float%20%28single-precision%29)))

(fn ConstructionScript)