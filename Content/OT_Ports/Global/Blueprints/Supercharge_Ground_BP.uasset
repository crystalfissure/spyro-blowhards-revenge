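; Supercharge ground trigger that starts Spyro's supercharge while he is on it.
; The static mesh's begin and end overlap events, filtered to Spyro's capsule component, track an overlap flag and cache the player reference.
; Each Tick while overlapping, it calls StartSupercharging if Spyro's player state matches a specific value and he is not already supercharging.
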(event OnComponentBeginOverlap(StaticMesh)
  (params (OverlappedComponent :type Primitive%20Component%20Object%20Reference) (OtherActor :type Actor%20Object%20Reference) (OtherComp :type Primitive%20Component%20Object%20Reference) (OtherBodyIndex :type Integer) (bFromSweep :type Boolean) (SweepResult :type Hit%20Result%20Structure%20%28by%20ref%29))
  (bind _asbp_spyro (Utilities|Casting|CastToBP_Spyro OtherActor))
  (if (== (Variables|/Script/Engine.Character|GetCapsuleComponent _asbp_spyro) OtherComp)
    (Variables|Default|SetIs%20Overlapping true)
    (Variables|Default|SetAs%20BP%20Spyro _asbp_spyro)))

(event OnComponentEndOverlap(StaticMesh)
  (params (OverlappedComponent :type Primitive%20Component%20Object%20Reference) (OtherActor :type Actor%20Object%20Reference) (OtherComp :type Primitive%20Component%20Object%20Reference) (OtherBodyIndex :type Integer))
  (bind _asbp_spyro (Utilities|Casting|CastToBP_Spyro OtherActor))
  (if (== (Variables|/Script/Engine.Character|GetCapsuleComponent _asbp_spyro) OtherComp)
    (Variables|Default|SetIs%20Overlapping false)))

(event EventTick
  (params (DeltaSeconds :type Float%20%28single-precision%29))
  (if (Variables|Default|GetIs%20Overlapping)
    (if (Utilities|Enum|Equal(Enum) (Variables|/Game/SpyroContent/Global_Assets/Global_Characters/Playable_Characters/BP_Base_Playable.BP_Base_Playable_C|GetPlayer_State (Variables|Default|GetAs%20BP%20Spyro)) "NewEnumerator4")
      (if (not (Variables|/Game/SpyroContent/Global_Assets/Global_Characters/Playable_Characters/Spyro/BP_Spyro.BP_Spyro_C|Getis_Currently_Supercharging (Variables|Default|GetAs%20BP%20Spyro)))
        (Default|StartSupercharging (Variables|Default|GetAs%20BP%20Spyro))))))

(fn ConstructionScript)