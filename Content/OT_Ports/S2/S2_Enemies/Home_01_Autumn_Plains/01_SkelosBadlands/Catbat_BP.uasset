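; Catbat is a flying enemy for the Skelos Badlands level, built on walking and flying AI components plus Damageable.
; Walking AI state changes are mirrored to the flying AI and drive gravity, which is off while idle, alert or attacking and on when dying so it falls.
; Melting from ice or ceasing to be afraid, both Damageable events, immediately stops its movement.
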(event Custom|Character%20state%20changed
  (bind _walking_ai_character (Variables|Default|GetWalking_AI_Character))
  (bind _charactermovement (Variables|Character|GetCharacterMovement))
  (bind _aicharacter_state (Variables|/Game/SpyroContent/Global_Assets/Global_Components/Base_AI_Character.Base_AI_Character_C|GetAICharacter_State _walking_ai_character))
  (Default|ChangeAICharacterState (Variables|Default|GetFlying_AI_Character) _aicharacter_state)
  (switch Utilities|FlowControl|Switch|SwitchonAICharacter_States _aicharacter_state
    (:NewEnumerator0
      (Variables|/Script/Engine.CharacterMovementComponent|SetGravityScale _charactermovement 0.0 :!label _label))
    (:NewEnumerator1
      (goto _label))
    (:NewEnumerator2
      (goto _label))
    (:NewEnumerator3
      (Variables|/Script/Engine.CharacterMovementComponent|SetGravityScale _charactermovement 1.5))))

(event Custom|Character%20melted
  (Components|Movement|StopMovementImmediately (Variables|Character|GetCharacterMovement)))

(event EventBeginPlay
  (|CallParentFunction)
  (EventDispatchers|BindEventtoMyStateChanged (Variables|Default|GetWalking_AI_Character) (delegate Custom|Character%20state%20changed))
  (EventDispatchers|BindEventtoMeltedfromIce (Variables|Default|GetDamageable) (delegate Custom|Character%20melted))
  (EventDispatchers|BindEventtoCallStopBeingAfraid (Variables|Default|GetDamageable) (delegate Custom|Character%20melted)))

(event Collision|EventActorBeginOverlap
  (params (OtherActor :type Actor%20Object%20Reference))
  (|CallParentFunction OtherActor) ; This node is disabled and will not be called.\nDrag off pins to build functionality.
)

(event EventTick
  (params (DeltaSeconds :type Float%20%28single-precision%29))
  (|CallParentFunction DeltaSeconds) ; This node is disabled and will not be called.\nDrag off pins to build functionality.
)

(fn ConstructionScript
  (|CallParentFunction))