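; Indigo Lizard enemy Blueprint for the Glimmer level of Summer Forest, a child class that leaves nearly all behavior to its parent.
; On BeginPlay it runs the parent logic, then resizes the AttackRadius sphere from a fixed base radius multiplied by AlertRadiusScale, updating overlaps.
; The construction script only calls the parent, and the Tick and overlap events are disabled placeholders.
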(event EventBeginPlay
  (|CallParentFunction)
  (Components|Sphere|SetSphereRadius (Variables|Default|GetAttack_Radius) (* 3e+02 (Variables|Default|GetAlert%20Radius%20Scale)) true))

(event Collision|EventActorBeginOverlap
  (params (OtherActor :type Actor%20Object%20Reference))
  (|CallParentFunction OtherActor) ; This node is disabled and will not be called.\nDrag off pins to build functionality.
)

(event EventTick
  (params (DeltaSeconds :type Float%20%28single-precision%29))
  (|CallParentFunction DeltaSeconds) ; This node is disabled and will not be called.\nDrag off pins to build functionality.
)

(fn ConstructionScript
  (|CallParentFunction))