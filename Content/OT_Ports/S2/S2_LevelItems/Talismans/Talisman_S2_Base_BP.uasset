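; Base actor for Spyro 2 talismans and spell ingredients awarded by NPCs: plays the reward cutscene for a spinning collectible.
; BeginPlay flags duplicates with a widget, saves the collectible, shows chimes and fireworks, then opens level completion UI and self-destructs.
; NPCRewardProcess blends the view to the talisman and pauses music; timers or skip inputs restore control.
; Boat-part and spell-ingredient counters queue story cutscenes at three, but their calls are disconnected.
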(event Custom|Look%20at%20me
  (Utilities|FlowControl|Delay 0.5)
  (if (not (Variables|Default|GetCutscene%20Was%20Skipped))
    (bind _player_who_was_awarded_me (Variables|/Game/SpyroContent/Global_Assets/Global_Components/NPC_Award_Item.NPC_Award_Item_C|GetPlayer%20Who%20Was%20Awarded%20Me (Variables|Default|GetNPC_Award_Item))
      (:then
        (Variables|/Game/SpyroContent/Global_Assets/Global_Characters/Playable_Characters/BP_Base_Playable.BP_Base_Playable_C|SetLookAt_Target _player_who_was_awarded_me (Variables|Default|GetStaticMesh)))
      (:else))))

(event Custom|Delayed%20Hide%20Black%20Bars
  (Utilities|FlowControl|Delay 3.0)
  (Utilities|FlowControl|DoOnce false
    (:Completed
      (bind _player_who_was_awarded_me (Variables|/Game/SpyroContent/Global_Assets/Global_Components/NPC_Award_Item.NPC_Award_Item_C|GetPlayer%20Who%20Was%20Awarded%20Me (Variables|Default|GetNPC_Award_Item))
        (:then
          (Default|HideBlackBars (Variables|/Game/SpyroContent/Global_Assets/Global_Characters/Playable_Characters/BP_Base_Playable.BP_Base_Playable_C|GetSpyroContr_Ref _player_who_was_awarded_me))
          (Game|Player|SetViewTargetwithBlend (Variables|/Game/SpyroContent/Global_Assets/Global_Characters/Playable_Characters/BP_Base_Playable.BP_Base_Playable_C|GetSpyroContr_Ref _player_who_was_awarded_me) _player_who_was_awarded_me 1.0 "VTBlend_Linear" 0.0 false)
          (Variables|/Game/SpyroContent/Global_Assets/Global_Characters/Playable_Characters/BP_Base_Playable.BP_Base_Playable_C|SetLookAt_Target _player_who_was_awarded_me 0)
          (Utilities|FlowControl|Delay 0.5)
          (CallFunction|Pause/UnpauseMusic self false false)
          (CallFunction|ImmediateRegainControl))
        (:else
          (Development|PrintString "Boat Part Base BP: cant regain control because the player who was awarded me ref is invalid"))))))

(event Custom|Reset%20Players%20Camera
  (Utilities|FlowControl|Delay 1.1)
  (if (not (Variables|Default|GetCutscene%20Was%20Skipped))
    (bind _player_who_was_awarded_me (Variables|/Game/SpyroContent/Global_Assets/Global_Components/NPC_Award_Item.NPC_Award_Item_C|GetPlayer%20Who%20Was%20Awarded%20Me (Variables|Default|GetNPC_Award_Item))
      (:then
        (Default|InvokedResetCamera _player_who_was_awarded_me))
      (:else))))

(event Custom|NPC%20Reward%20Process
  (Utilities|FlowControl|Delay 0.1)
  (bind _player_who_was_awarded_me (Variables|/Game/SpyroContent/Global_Assets/Global_Components/NPC_Award_Item.NPC_Award_Item_C|GetPlayer%20Who%20Was%20Awarded%20Me (Variables|Default|GetNPC_Award_Item))
    (:then
      (CallFunction|Pause/UnpauseMusic self true false)
      (CallFunction|DisableThisPlayer'sInputs _player_who_was_awarded_me)
      (Input|EnableInput (Variables|/Game/SpyroContent/Global_Assets/Global_Characters/Playable_Characters/BP_Base_Playable.BP_Base_Playable_C|GetSpyroContr_Ref _player_who_was_awarded_me))
      (CallFunction|LookatMe)
      (Camera|SetFieldOfView (Variables|Default|GetCamera) (Variables|/Script/Engine.CameraComponent|GetFieldOfView (Variables|/Game/SpyroContent/Global_Assets/Global_Characters/Playable_Characters/BP_Base_Playable.BP_Base_Playable_C|GetFollowCamera _player_who_was_awarded_me)))
      (Game|Player|SetViewTargetwithBlend (Variables|/Game/SpyroContent/Global_Assets/Global_Characters/Playable_Characters/BP_Base_Playable.BP_Base_Playable_C|GetSpyroContr_Ref _player_who_was_awarded_me) self 1.5 "VTBlend_Linear" 0.0 false)
      (CallFunction|DelayedHideBlackBars)
      (CallFunction|ResetPlayersCamera))
    (:else)))

(event Custom|Immediate%20Regain%20Control
  (Utilities|FlowControl|DoOnce false
    (:Completed
      (bind _player_who_was_awarded_me (Variables|/Game/SpyroContent/Global_Assets/Global_Components/NPC_Award_Item.NPC_Award_Item_C|GetPlayer%20Who%20Was%20Awarded%20Me (Variables|Default|GetNPC_Award_Item))
        (:then
          (Variables|/Game/SpyroContent/Global_Assets/Global_Characters/Playable_Characters/BP_Base_Playable.BP_Base_Playable_C|GetTalking_NPC _player_who_was_awarded_me
            (:then
              _)
            (:else
              (Input|EnableInput _player_who_was_awarded_me (Variables|/Game/SpyroContent/Global_Assets/Global_Characters/Playable_Characters/BP_Base_Playable.BP_Base_Playable_C|GetSpyroContr_Ref _player_who_was_awarded_me))
              (Variables|/Game/SpyroContent/Global_Assets/Global_Characters/Playable_Characters/BP_Base_Playable.BP_Base_Playable_C|SetDid%20we%20disable%20input? _player_who_was_awarded_me false)))
          (Input|DisableInput (Variables|/Game/SpyroContent/Global_Assets/Global_Characters/Playable_Characters/BP_Base_Playable.BP_Base_Playable_C|GetSpyroContr_Ref _player_who_was_awarded_me)))
        (:else
          _))
      (CallFunction|DelayedEnableInput)
      (bind _npc_who_awarded_me (Variables|/Game/SpyroContent/Global_Assets/Global_Components/NPC_Award_Item.NPC_Award_Item_C|GetNPC%20Who%20Awarded%20Me (Variables|Default|GetNPC_Award_Item))
        (:then
          (Variables|/Game/SpyroContent/Global_Assets/Global_Characters/NPCs/NPC_Base_BP.NPC_Base_BP_C|SetItem%20Award%20is%20Happening _npc_who_awarded_me false))
        (:else
          _))
      (bind _foundwidgets (Widget|GetAllWidgetsOfClass "/Game/SpyroContent/Global_Assets/Global_UserInterface/Widgets/YouAlreadyHaveThisX.YouAlreadyHaveThisX_C" true))
      (Utilities|IsValid (Utilities|Array|Get(acopy) _foundwidgets)
        (:Is%20Valid
          (Widget|RemovefromParent (Utilities|Array|Get(acopy) _foundwidgets)))))))

(event Custom|Delayed%20Enable%20Input
  (Utilities|FlowControl|Delay 0.5)
  (bind _player_who_was_awarded_me (Variables|/Game/SpyroContent/Global_Assets/Global_Components/NPC_Award_Item.NPC_Award_Item_C|GetPlayer%20Who%20Was%20Awarded%20Me (Variables|Default|GetNPC_Award_Item))
    (:then
      (Variables|/Game/SpyroContent/Global_Assets/Global_Characters/Playable_Characters/BP_Base_Playable.BP_Base_Playable_C|GetTalking_NPC _player_who_was_awarded_me
        (:then)
        (:else
          (Input|EnableInput _player_who_was_awarded_me (Variables|/Game/SpyroContent/Global_Assets/Global_Characters/Playable_Characters/BP_Base_Playable.BP_Base_Playable_C|GetSpyroContr_Ref _player_who_was_awarded_me))
          (Variables|/Game/SpyroContent/Global_Assets/Global_Characters/Playable_Characters/BP_Base_Playable.BP_Base_Playable_C|SetDid%20we%20disable%20input? _player_who_was_awarded_me false))))
    (:else)))

(event Custom|Immediate%20Hide%20Black%20Bars
  (Utilities|FlowControl|DoOnce false
    (:Completed
      (bind _player_who_was_awarded_me (Variables|/Game/SpyroContent/Global_Assets/Global_Components/NPC_Award_Item.NPC_Award_Item_C|GetPlayer%20Who%20Was%20Awarded%20Me (Variables|Default|GetNPC_Award_Item))
        (:then
          (Default|HideBlackBars (Variables|/Game/SpyroContent/Global_Assets/Global_Characters/Playable_Characters/BP_Base_Playable.BP_Base_Playable_C|GetSpyroContr_Ref _player_who_was_awarded_me))
          (Game|Player|SetViewTargetwithBlend (Variables|/Game/SpyroContent/Global_Assets/Global_Characters/Playable_Characters/BP_Base_Playable.BP_Base_Playable_C|GetSpyroContr_Ref _player_who_was_awarded_me) _player_who_was_awarded_me 1.0 "VTBlend_Linear" 0.0 false)
          (Variables|/Game/SpyroContent/Global_Assets/Global_Characters/Playable_Characters/BP_Base_Playable.BP_Base_Playable_C|SetLookAt_Target _player_who_was_awarded_me 0)
          (Utilities|FlowControl|Delay 0.5)
          (CallFunction|Pause/UnpauseMusic self false false)
          (CallFunction|ImmediateRegainControl))
        (:else
          (Development|PrintString "Boat Part Base BP: cant regain control because the player who was awarded me ref is invalid"))))))

(event EventBeginPlay
  (bind _staticmesh (Variables|Default|GetStaticMesh))
  (|Checkifwealreadyhavethis
    (:then_1
      (bind _asspyro_persistant_data (Utilities|Casting|CastToSpyro_PersistantData (Game|GetGameInstance))
        (:then
          (Default|SaveACollectible _asspyro_persistant_data "NewEnumerator3" "" 0.0 0 2.0))
        (:CastFailed
          _))
      (CallFunction|NPCRewardProcess)
      (Utilities|FlowControl|Delay 1.0)
      (Components|Activation|Activate (Variables|Default|GetAppear_ParticleSystem) false)
      (Audio|PlaySoundatLocation "/Game/SpyroContent/CiC_Assets/CiC_Level_Items/Boat/talisman_chime_truncated.talisman_chime_truncated" (Transformation|GetWorldLocation (Variables|Default|GetStaticMesh)) "0, 0, 0" 1.0 1.0 0.0 0 0 0)
      (Utilities|FlowControl|Delay 0.2)
      (Development|SetHiddeninGame (Variables|Default|GetStaticMesh) false true)
      (Utilities|FlowControl|Delay 1.5)
      (Effects|SpawnEmitteratLocation "/Game/SpyroContent/CiC_Assets/CiC_Level_Items/Dragon_Candle/PS_Fireworks_Burst.PS_Fireworks_Burst" (Transformation|GetWorldLocation (Variables|Default|GetStaticMesh)))
      (Development|SetHiddeninGame _staticmesh true true)
      (Audio|PlaySoundatLocation "/Game/SpyroContent/CiC_Assets/CiC_Level_Items/Boat/talisman_chime_truncated.talisman_chime_truncated" (Transformation|GetWorldLocation _staticmesh) "0, 0, 0" 1.0 1.0 0.0 0 0 0)
      (Utilities|FlowControl|Delay 1.5)
      (bind _returnvalue (UserInterface|CreateWidget "/Game/SpyroContent/Global_Assets/Global_UserInterface/Widgets/Level_Completion_UI.Level_Completion_UI_C"))
      (UserInterface|Viewport|AddtoViewport _returnvalue 0)
      (Actor|DestroyActor))))

(event EventTick
  (params (DeltaSeconds :type Float%20%28single-precision%29))
  (Transformation|AddLocalRotation (Variables|Default|GetStaticMesh) (Math|Rotator|MakeRotator 0.0 0.0 (* DeltaSeconds -1.6e+02)) false false))

(event Input|ActionEvents|InputActionPause
  (params (Key :type Key%20Structure :default "None"))
  (:Pressed
    (Utilities|FlowControl|DoOnce false
      (:Completed
        (Variables|Default|SetCutscene%20Was%20Skipped true)
        (CallFunction|ImmediateRegainControl)
        (CallFunction|ImmediateHideBlackBars)))))

(event Input|ActionEvents|InputActionAim/Talk
  (params (Key :type Key%20Structure :default "None"))
  (:Pressed
    (Utilities|FlowControl|DoOnce false
      (:Completed
        (Variables|Default|SetCutscene%20Was%20Skipped true)
        (CallFunction|ImmediateRegainControl)
        (CallFunction|ImmediateHideBlackBars)))))

(event Input|KeyboardEvents|SpaceBar
  (params (Key :type Key%20Structure :default "None"))
  (:Pressed
    (Utilities|FlowControl|DoOnce false
      (:Completed
        (Variables|Default|SetCutscene%20Was%20Skipped true)
        (CallFunction|ImmediateRegainControl)
        (CallFunction|ImmediateHideBlackBars)))))

(event Input|MouseEvents|LeftMouseButton
  (params (Key :type Key%20Structure :default "None"))
  (:Pressed
    (Utilities|FlowControl|DoOnce false
      (:Completed
        (Variables|Default|SetCutscene%20Was%20Skipped true)
        (CallFunction|ImmediateRegainControl)
        (CallFunction|ImmediateHideBlackBars)))))

(fn ConstructionScript)

(fn CountBoatParts
  (params (WorldContextObject :type Object%20Object%20Reference))
  (Utilities|FlowControl|Sequence
    (:then_0
      (LocalVariables|SetTotal 0)
      (bind _returnvalue (CallFunction|DoWeHaveThisTalisman? WorldContextObject 0 1 WorldContextObject))
      (if _returnvalue
        (Math|Integer|IncrementInt (LocalVariables|GetTotal))))
    (:then_1
      (bind _returnvalue_2 (CallFunction|DoWeHaveThisTalisman? WorldContextObject 0 3 WorldContextObject))
      (if _returnvalue_2
        (Math|Integer|IncrementInt (LocalVariables|GetTotal))))
    (:then_2
      (bind _returnvalue_3 (CallFunction|DoWeHaveThisTalisman? WorldContextObject 0 2 WorldContextObject))
      (if _returnvalue_3
        (Math|Integer|IncrementInt (LocalVariables|GetTotal))))
    (:then_3
      (bind _returnvalue_4 (CallFunction|DoWeHaveThisTalisman? WorldContextObject 0 4 WorldContextObject))
      (if _returnvalue_4
        (Math|Integer|IncrementInt (LocalVariables|GetTotal))))
    (:then_4
      (bind _returnvalue_5 (CallFunction|DoWeHaveThisTalisman? WorldContextObject 0 7 WorldContextObject))
      (if _returnvalue_5
        (Math|Integer|IncrementInt (LocalVariables|GetTotal))))
    (:then_5
      (if (== (LocalVariables|GetTotal) 3)
        (bind (_asspyro_save_data _as_persistent_data _slot_name) (CallFunction|LoadSpyroGame WorldContextObject 0 WorldContextObject))
        (Variables|/Game/SpyroContent/Global_Assets/Global_SaveData/Spyro_SaveData.Spyro_SaveData_C|SetIncoming_Cutscene _asspyro_save_data "/Game/SpyroContent/CiC_Assets/CiC_Levels/CiC_Cutscenes/CiC_Cutscene_02_Spyro_and_Elora.CiC_Cutscene_02_Spyro_and_Elora")
        (SaveGame|SaveGametoSlot _asspyro_save_data _slot_name)
        (Development|PrintString WorldContextObject "THE CUTSCENE IS ALL SET" true true "(R=0.000000,G=0.660000,B=1.000000,A=1.000000)" 3e+01)
        (else
          (Development|PrintString WorldContextObject (Utilities|String|Append "I COUNTED, YOU HAVE " (Utilities|String|ToString(Integer) (LocalVariables|GetTotal))) true true "(R=0.000000,G=0.660000,B=1.000000,A=1.000000)" 3e+01))))
    (:then_6
      (return))))

(fn CountSpellIngredients
  (params (WorldContextObject :type Object%20Object%20Reference))
  (Utilities|FlowControl|Sequence
    (:then_0
      (LocalVariables|SetTotal 0)
      (bind _returnvalue (CallFunction|DoWeHaveThisTalisman? WorldContextObject 1 1 WorldContextObject))
      (if _returnvalue
        (Math|Integer|IncrementInt (LocalVariables|GetTotal))))
    (:then_1
      (bind _returnvalue_2 (CallFunction|DoWeHaveThisTalisman? WorldContextObject 1 2 WorldContextObject))
      (if _returnvalue_2
        (Math|Integer|IncrementInt (LocalVariables|GetTotal))))
    (:then_2
      (bind _returnvalue_3 (CallFunction|DoWeHaveThisTalisman? WorldContextObject 1 3 WorldContextObject))
      (if _returnvalue_3
        (Math|Integer|IncrementInt (LocalVariables|GetTotal))))
    (:then_3
      (bind _returnvalue_4 (CallFunction|DoWeHaveThisTalisman? WorldContextObject 1 4 WorldContextObject))
      (if _returnvalue_4
        (Math|Integer|IncrementInt (LocalVariables|GetTotal))))
    (:then_4
      (if (== (LocalVariables|GetTotal) 3)
        (bind (_asspyro_save_data _as_persistent_data _slot_name) (CallFunction|LoadSpyroGame WorldContextObject 0 WorldContextObject))
        (Variables|/Game/SpyroContent/Global_Assets/Global_SaveData/Spyro_SaveData.Spyro_SaveData_C|SetIncoming_Cutscene _asspyro_save_data "/Game/SpyroContent/CiC_Assets/CiC_Levels/CiC_Cutscenes/CiC_Cutscene_04_Hunter_and_Bianca.CiC_Cutscene_04_Hunter_and_Bianca")
        (SaveGame|SaveGametoSlot _asspyro_save_data _slot_name)
        (Development|PrintString WorldContextObject "THE CUTSCENE IS ALL SET" true true "(R=0.000000,G=0.660000,B=1.000000,A=1.000000)" 3e+01)
        (else
          (Development|PrintString WorldContextObject (Utilities|String|Append "I COUNTED, YOU HAVE " (Utilities|String|ToString(Integer) (LocalVariables|GetTotal))) true true "(R=0.000000,G=0.660000,B=1.000000,A=1.000000)" 3e+01))))
    (:then_5
      (return))))