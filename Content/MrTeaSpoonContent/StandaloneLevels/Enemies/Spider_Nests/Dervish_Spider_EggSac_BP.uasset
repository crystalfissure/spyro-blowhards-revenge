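; Destructible spider egg sac nest that spawns Dervish spiders once a player capsule first enters its alert radius, and again on container reset.
; After a difficulty-scaled delay, an intact sac replaces its previous spider with a tiny one that it launches forward, triggers to grow and links back to itself, with squash-stretch and sound.
; Difficulty comes from the universal save, using saved skill level when Dynamic, and refreshes on change.
; Successful damage plays a burst effect.
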(event OnComponentBeginOverlap(AlertRadius)
  (params (OverlappedComponent :type Primitive%20Component%20Object%20Reference) (OtherActor :type Actor%20Object%20Reference) (OtherComp :type Primitive%20Component%20Object%20Reference) (OtherBodyIndex :type Integer) (bFromSweep :type Boolean) (SweepResult :type Hit%20Result%20Structure%20%28by%20ref%29))
  (bind _asbp_base_playable (Utilities|Casting|CastToBP_Base_Playable OtherActor))
  (if (== (Variables|/Script/Engine.Character|GetCapsuleComponent _asbp_base_playable) OtherComp)
    (Utilities|FlowControl|DoOnce false
      (:Completed
        (CallFunction|SpawnDragoid)))))

(event DamageWasSuccessfullyDealt(Damageable)
  (bind _staticmesh (Variables|Default|GetStaticMesh))
  (bind _returnvalue (Transformation|GetWorldTransform _staticmesh))
  (bind (_location _rotation) (Math|Transform|BreakTransform _returnvalue))
  (Effects|SpawnEmitteratLocation "/Game/MrTeaSpoonContent/StandaloneLevels/Enemies/Egg_Sacs/eggsac_burst.eggsac_burst" _location _rotation "3.500000,3.500000,3.500000"))

(event Custom|Spawn%20Dragoid
  (bind _medium (Variables|Default|GetMedium))
  (if (not (Variables|Default|GetContainer_Destroyed))
    (Utilities|FlowControl|Delay (Utilities|Select :Index (Variables|Default|GetMy%20Current%20Difficulty) :NewEnumerator4 _medium :NewEnumerator0 (Variables|Default|GetEasy) :NewEnumerator1 _medium :NewEnumerator2 (Variables|Default|GetHard) :NewEnumerator3 (Variables|Default|GetNightmare)))
    (if (not (Variables|Default|GetContainer_Destroyed))
      (bind _my_dragoid (Variables|Default|GetMy%20Dragoid)
        (:then
          (Actor|DestroyActor _my_dragoid))
        (:else
          _))
      (bind _returnvalue (Game|SpawnActorfromClass "/Game/MrTeaSpoonContent/StandaloneLevels/Enemies/Spiders/Dervish_Spider_BP.Dervish_Spider_BP_C" (Math|Transform|MakeTransform (Transformation|GetWorldLocation (Variables|Default|Getspawn%20point)) (Math|Rotator|MakeRotator 0.0 0.0 (.yaw (Transformation|GetActorRotation))) "0.100000,0.100000,0.100000") "AdjustIfPossibleButAlwaysSpawn" 0 0))
      (Variables|/Game/MrTeaSpoonContent/StandaloneLevels/Enemies/Spiders/Dervish_Spider_BP.Dervish_Spider_BP_C|Setspawned%20from%20nest _returnvalue true)
      (Variables|Default|SetMy%20Dragoid _returnvalue)
      (Default|GrowthSpurt _returnvalue)
      (Variables|/Game/MrTeaSpoonContent/StandaloneLevels/Enemies/Spiders/Dervish_Spider_BP.Dervish_Spider_BP_C|SetMy%20Nest _returnvalue self)
      (Character|LaunchCharacter _returnvalue (+ (* (Transformation|GetActorForwardVector) (Variables|Default|Getforward%20launch)) (* (Transformation|GetActorUpVector) 2e+02)) false false)
      (Audio|PlaySoundatLocation "/Game/SpyroContent/Global_Assets/Global_Level_Items/Spittable_Object/LavaRock/lava_rock_spit.lava_rock_spit" (Transformation|GetActorLocation) "0, 0, 0" 1.0 0.5 0.0 0 0 0)
      (bind (_direction _newtrack_0 _newtrack_1) (Timeline|Squish%20&%20Stretch PlayFromStart)
        (:Update
          (Transformation|SetRelativeScale3D (Variables|Default|GetStaticMesh) (Math|Vector|MakeVector _newtrack_0 _newtrack_1 _newtrack_1)))))))

(event Custom|Set%20My%20Difficulty
  (bind _asspyro_universal_save_data (CallFunction|LoadUniversalSave))
  (if (Utilities|Enum|Equal(Enum) (Variables|/Game/SpyroContent/Global_Assets/Global_SaveData/Spyro_Universal_Save_Data.Spyro_Universal_Save_Data_C|GetDifficulty _asspyro_universal_save_data) "NewEnumerator4")
    (bind _asspyro_save_data (CallFunction|LoadSpyroGame self))
    (bind _difficulty (CallFunction|ConvertSkillLevelFloattoEnum (Variables|/Game/SpyroContent/Global_Assets/Global_SaveData/Spyro_SaveData.Spyro_SaveData_C|GetSkill_Level _asspyro_save_data)))
    (Variables|Default|SetMy%20Current%20Difficulty _difficulty)
    (else
      (Variables|Default|SetMy%20Current%20Difficulty (Variables|/Game/SpyroContent/Global_Assets/Global_SaveData/Spyro_Universal_Save_Data.Spyro_Universal_Save_Data_C|GetDifficulty _asspyro_universal_save_data)))))

(event EventBeginPlay
  (|CallParentFunction)
  (bind _asspyro_persistant_data (Utilities|Casting|CastToSpyro_PersistantData (Game|GetGameInstance))
    (:then
      (EventDispatchers|BindEventtoDifficultyChanged _asspyro_persistant_data (delegate Custom|Set%20My%20Difficulty)))
    (:CastFailed
      _))
  (CallFunction|SetMyDifficulty))

(event EventResetThisContainer
  (|CallParentFunction)
  (CallFunction|SpawnDragoid))

(fn ConstructionScript
  (|CallParentFunction))