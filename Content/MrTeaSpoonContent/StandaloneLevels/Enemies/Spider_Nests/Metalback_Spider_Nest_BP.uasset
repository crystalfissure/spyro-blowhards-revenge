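; Destructible metalback spider nest that launches a small metal spider from its spawn point, provided it is intact and spawning is enabled.
; BeginPlay and container reset trigger SpawnDragoid, which waits a difficulty-based delay, replaces any existing spider, then links the new one to the nest and triggers its growth spurt.
; Difficulty comes from the universal save, or the player's saved skill level when Dynamic, and refreshes on difficulty changes.
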(event Custom|Spawn%20Dragoid
  (bind _medium (Variables|Default|GetMedium))
  (if (not (Variables|Default|GetContainer_Destroyed))
    (if (Variables|Default|GetSpawnAtBeginPlay)
      (Utilities|FlowControl|Delay (Utilities|Select :Index (Variables|Default|GetMy%20Current%20Difficulty) :NewEnumerator4 _medium :NewEnumerator0 (Variables|Default|GetEasy) :NewEnumerator1 _medium :NewEnumerator2 (Variables|Default|GetHard) :NewEnumerator3 (Variables|Default|GetNightmare)))
      (if (not (Variables|Default|GetContainer_Destroyed))
        (bind _my_dragoid (Variables|Default|GetMy%20Dragoid)
          (:then
            (Actor|DestroyActor _my_dragoid))
          (:else
            _))
        (bind _returnvalue (Game|SpawnActorfromClass "/Game/MrTeaSpoonContent/StandaloneLevels/Enemies/Spiders/Metal_Spider_Smaller_BP.Metal_Spider_Smaller_BP_C" (Math|Transform|MakeTransform (Transformation|GetWorldLocation (Variables|Default|Getspawn%20point)) (Math|Rotator|MakeRotator 0.0 0.0 (.yaw (Transformation|GetActorRotation))) "0.100000,0.100000,0.100000") "AdjustIfPossibleButAlwaysSpawn" 0 0))
        (Variables|/Game/MrTeaSpoonContent/StandaloneLevels/Enemies/Spiders/Metal_Spider_BP.Metal_Spider_BP_C|Setspawned%20from%20nest _returnvalue true)
        (bind _output_get (Variables|Default|SetMy%20Dragoid _returnvalue))
        (Default|GrowthSpurt _output_get)
        (Variables|/Game/MrTeaSpoonContent/StandaloneLevels/Enemies/Spiders/Metal_Spider_BP.Metal_Spider_BP_C|SetMy%20Nest _returnvalue self)
        (Character|LaunchCharacter _returnvalue (+ (* (Transformation|GetActorForwardVector) (Variables|Default|Getforward%20launch)) (* (Transformation|GetActorUpVector) 2e+02)) false false)
        (Audio|PlaySoundatLocation "/Game/SpyroContent/Global_Assets/Global_Level_Items/Spittable_Object/LavaRock/lava_rock_spit.lava_rock_spit" (Transformation|GetActorLocation) "0, 0, 0" 1.0 0.5 0.0 0 0 0)))))

(event Custom|Set%20My%20Difficulty
  (bind _asspyro_universal_save_data (CallFunction|LoadUniversalSave))
  (if (Utilities|Enum|Equal(Enum) (Variables|/Game/SpyroContent/Global_Assets/Global_SaveData/Spyro_Universal_Save_Data.Spyro_Universal_Save_Data_C|GetDifficulty _asspyro_universal_save_data) "NewEnumerator4")
    (bind _asspyro_save_data (CallFunction|LoadSpyroGame self))
    (bind _difficulty (CallFunction|ConvertSkillLevelFloattoEnum (Variables|/Game/SpyroContent/Global_Assets/Global_SaveData/Spyro_SaveData.Spyro_SaveData_C|GetSkill_Level _asspyro_save_data)))
    (Variables|Default|SetMy%20Current%20Difficulty _difficulty)
    (else
      (Variables|Default|SetMy%20Current%20Difficulty (Variables|/Game/SpyroContent/Global_Assets/Global_SaveData/Spyro_Universal_Save_Data.Spyro_Universal_Save_Data_C|GetDifficulty _asspyro_universal_save_data)))))

(event EventBeginPlay
  (|CallParentFunction)
  (CallFunction|SpawnDragoid)
  (bind _asspyro_persistant_data (Utilities|Casting|CastToSpyro_PersistantData (Game|GetGameInstance))
    (:then
      (EventDispatchers|BindEventtoDifficultyChanged _asspyro_persistant_data (delegate Custom|Set%20My%20Difficulty)))
    (:CastFailed
      _))
  (CallFunction|SetMyDifficulty))

(event EventResetThisContainer
  (|CallParentFunction)
  (CallFunction|SpawnDragoid))

(fn ConstructionScript
  (|CallParentFunction))