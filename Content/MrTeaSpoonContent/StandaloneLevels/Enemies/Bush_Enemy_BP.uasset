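; Killer bush enemy that lunges from its spawn point to swallow players, returning home if it misses.
; WalkingAICharacter state changes swap mesh and AnimBP and drive timeline lunge and return, with a difficulty-based re-alert delay.
; A looping box trace and EatingArea overlaps catch players, disabling input, hiding them and blending to the bush camera.
; Dying releases the player and bursts into leaves, leaving a burned hedge for one damage type.
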(event OnComponentBeginOverlap(EatingArea)
  (params (OverlappedComponent :type Primitive%20Component%20Object%20Reference) (OtherActor :type Actor%20Object%20Reference) (OtherComp :type Primitive%20Component%20Object%20Reference) (OtherBodyIndex :type Integer) (bFromSweep :type Boolean) (SweepResult :type Hit%20Result%20Structure%20%28by%20ref%29))
  (bind _asstatic_bush_bp (Utilities|Casting|CastToStaticBush_BP OtherActor)
    (:then
      (if (and (Utilities|Enum|Equal(Enum) (Variables|/Game/SpyroContent/Global_Assets/Global_Components/Base_AI_Character.Base_AI_Character_C|GetAICharacter_State (Variables|Default|GetWalking_AI_Character)) "NewEnumerator2") (== (Variables|/Game/MrTeaSpoonContent/StandaloneLevels/Objects/StaticBush_BP.StaticBush_BP_C|GetCapsule _asstatic_bush_bp) OtherComp))
        (Default|DealDamage (Variables|/Game/MrTeaSpoonContent/StandaloneLevels/Objects/StaticBush_BP.StaticBush_BP_C|GetDamageable_Com _asstatic_bush_bp) "NewEnumerator4" "0, 0, 0" false 0 false)
        (CallFunction|CanIEatThisPlayer? OtherActor OtherComp :!label _label)))
    (:CastFailed
      (goto _label))))

(event Custom|On%20Bush%20Reset
  (bind _capsulecomponent (Variables|Default|GetCapsuleComponent))
  (bind _box_col (Variables|Default|GetBox_COL))
  (Collision|SetCollisionResponsetoChannel _box_col "ECC_Camera" "ECR_Block")
  (Collision|SetCollisionResponsetoChannel _box_col "ECC_Pawn" "ECR_Block")
  (Collision|SetCollisionResponsetoChannel _box_col "ECC_GameTraceChannel4" "ECR_Block")
  (Collision|SetCollisionResponsetoChannel _box_col "ECC_GameTraceChannel2" "ECR_Block")
  (Collision|SetCollisionResponsetoChannel _box_col "ECC_GameTraceChannel5" "ECR_Block")
  (Variables|/Game/SpyroContent/Global_Assets/Global_Components/Base_AI_Character.Base_AI_Character_C|SetCan_Become_Alert (Variables|Default|GetWalking_AI_Character) true)
  (Collision|SetCollisionObjectType _capsulecomponent "ECC_PhysicsBody")
  (Collision|SetCollisionResponsetoAllChannels _capsulecomponent "ECR_Ignore"))

(event Custom|Hedge%20State%20Changed
  (bind _returnvalue (Transformation|GetActorTransform))
  (bind _mesh (Variables|Character|GetMesh))
  (bind _mesh_2 (Variables|Character|GetMesh))
  (bind _damageable (Variables|Default|GetDamageable))
  (bind _mesh_3 (Variables|Character|GetMesh))
  (bind _mesh_4 (Variables|Character|GetMesh))
  (bind _returnvalue_2 (Components|SkeletalMesh|GetAnimInstance _mesh_4))
  (Utilities|FlowControl|Sequence
    (:then_0
      (if (Utilities|Enum|Equal(Enum) (Variables|/Game/SpyroContent/Global_Assets/Global_Components/Base_AI_Character.Base_AI_Character_C|GetAICharacter_State (Variables|Default|GetWalking_AI_Character)) "NewEnumerator2")
        (Utilities|Time|ClearandInvalidateTimerbyHandle (Variables|Default|GetEating%20Ping%20Timer))
        (bind _returnvalue_3 (Utilities|Time|SetTimerbyFunctionName 0 "Eating Ping" 0.2 true))
        (Variables|Default|SetEating%20Ping%20Timer _returnvalue_3)
        (CallFunction|LungeForwards)
        (else
          (Variables|/Script/Engine.PrimitiveComponent|SetCanCharacterStepUpOn (Variables|Default|GetCapsuleComponent) "ECB_Yes")
          (Utilities|Time|ClearandInvalidateTimerbyHandle (Variables|Default|GetEating%20Ping%20Timer))
          (CallFunction|StopLungingForwards)
          (bind _askiller_bush_2_abp (Utilities|Casting|CastToKiller_Bush_2_ABP _returnvalue_2)
            (:then
              (Variables|/Game/MrTeaSpoonContent/StandaloneLevels/Enemies/Bush/Killer_Bush_2_ABP.Killer_Bush_2_ABP_C|SetisEating _askiller_bush_2_abp false))
            (:CastFailed
              (bind _askiller_bush_3_abp (Utilities|Casting|CastToKiller_Bush_3_ABP _returnvalue_2))
              (Variables|/Game/MrTeaSpoonContent/StandaloneLevels/Enemies/Bush/Killer_Bush_3_ABP.Killer_Bush_3_ABP_C|SetisEating _askiller_bush_3_abp false))))))
    (:then_1
      (switch Utilities|FlowControl|Switch|SwitchonAICharacter_States (Variables|/Game/SpyroContent/Global_Assets/Global_Components/Base_AI_Character.Base_AI_Character_C|GetAICharacter_State (Variables|Default|GetWalking_AI_Character))
        (:NewEnumerator0
          (Class|SkinnedMeshComponent|SetSkeletalMesh _mesh "/Game/MrTeaSpoonContent/StandaloneLevels/Enemies/Bush/Killer_Bush_2.Killer_Bush_2" true :!label _label)
          (Class|SkeletalMeshComponent|SetAnimClass _mesh_2 "/Game/MrTeaSpoonContent/StandaloneLevels/Enemies/Bush/Killer_Bush_2_ABP.Killer_Bush_2_ABP_C")
          (Transformation|SetRelativeScale3D _mesh_3 "0.500000,0.500000,0.500000")
          (bind _askiller_bush_2_abp_2 (Utilities|Casting|CastToKiller_Bush_2_ABP _returnvalue_2))
          (Default|RefreshAnimBP _askiller_bush_2_abp_2))
        (:NewEnumerator1
          (goto _label))
        (:NewEnumerator2
          (Class|SkinnedMeshComponent|SetSkeletalMesh _mesh "/Game/MrTeaSpoonContent/StandaloneLevels/Enemies/Bush/Killer_Bush_3.Killer_Bush_3" true)
          (Class|SkeletalMeshComponent|SetAnimClass _mesh_2 "/Game/MrTeaSpoonContent/StandaloneLevels/Enemies/Bush/Killer_Bush_3_ABP.Killer_Bush_3_ABP_C")
          (Transformation|SetRelativeScale3D _mesh_3 "1.000000,1.000000,1.000000")
          (bind _askiller_bush_3_abp_2 (Utilities|Casting|CastToKiller_Bush_3_ABP _returnvalue_2))
          (Default|RefreshAnimBP _askiller_bush_3_abp_2))
        (:NewEnumerator3
          (CallFunction|ReleasethePlayerinMyMouth)
          (Effects|SpawnEmitteratLocation "/Game/SpyroContent/CiC_Assets/CiC_Levels/Home_01_PresentMeadows/01_AstralUtopia/Actors/Hedge/Meshes/leaf_burst_PS.leaf_burst_PS" (.location _returnvalue) (.rotation _returnvalue))
          (if (and (Utilities|Enum|Equal(Enum) (Variables|/Game/SpyroContent/Global_Assets/Global_Components/Damageable_Com.Damageable_Com_C|GetDeal%20Damage%20-%20Damage%20Type _damageable) "NewEnumerator1") (not (Variables|/Game/SpyroContent/Global_Assets/Global_Components/Damageable_Com.Damageable_Com_C|GetDeal%20Damage%20-%20Super%20Damage _damageable)))
            (Game|SpawnActorfromClass "/Game/SpyroContent/CiC_Assets/CiC_Levels/Home_01_PresentMeadows/01_AstralUtopia/Actors/Hedge/Burned_Hedge_BP.Burned_Hedge_BP_C" (Transformation|GetActorTransform) "AlwaysSpawn" 0 0)))))))

(event Custom|return%20home
  (bind _damageable (Variables|Default|GetDamageable))
  (CallFunction|StopLungingForwards)
  (Utilities|FlowControl|Sequence
    (:then_0
      (bind _newtrack_0 (Timeline|Timeline_2 PlayFromStart)
        (:Update
          (if (and (not (Variables|/Game/SpyroContent/Global_Assets/Global_Components/Damageable_Com.Damageable_Com_C|GetFrozen _damageable)) (not (Variables|/Game/SpyroContent/Global_Assets/Global_Components/Damageable_Com.Damageable_Com_C|GetParalyzed_by_Fear _damageable)))
            (Transformation|SetActorLocation (Math|Vector|Lerp(Vector) (Transformation|GetActorLocation) (Variables|/Game/SpyroContent/Global_Assets/Global_Components/Base_AI_Character.Base_AI_Character_C|GetSpawn_Point (Variables|Default|GetWalking_AI_Character)) _newtrack_0) false false)))))
    (:then_1
      (Utilities|FlowControl|Delay (Utilities|Select :Index (Variables|Default|GetMy%20Current%20Difficulty) :NewEnumerator4 0.5 :NewEnumerator0 1.0 :NewEnumerator1 1.0 :NewEnumerator2 0.0 :NewEnumerator3 0.0))
      (if (not (Utilities|Enum|Equal(Enum) (Variables|/Game/SpyroContent/Global_Assets/Global_Components/Base_AI_Character.Base_AI_Character_C|GetAICharacter_State (Variables|Default|GetWalking_AI_Character)) "NewEnumerator2"))
        (Utilities|Array|Clear (Variables|/Game/SpyroContent/Global_Assets/Global_Components/Base_AI_Character.Base_AI_Character_C|GetPlayers_I_Am_Alert_To (Variables|Default|GetWalking_AI_Character)))
        (Variables|/Game/SpyroContent/Global_Assets/Global_Components/Base_AI_Character.Base_AI_Character_C|SetCan_Become_Alert (Variables|Default|GetWalking_AI_Character) true)))))

(event Custom|stop%20returning%20home
  (bind _damageable (Variables|Default|GetDamageable))
  (bind _newtrack_0 (Timeline|Timeline_2 Stop)
    (:Update
      (if (and (not (Variables|/Game/SpyroContent/Global_Assets/Global_Components/Damageable_Com.Damageable_Com_C|GetFrozen _damageable)) (not (Variables|/Game/SpyroContent/Global_Assets/Global_Components/Damageable_Com.Damageable_Com_C|GetParalyzed_by_Fear _damageable)))
        (Transformation|SetActorLocation (Math|Vector|Lerp(Vector) (Transformation|GetActorLocation) (Variables|/Game/SpyroContent/Global_Assets/Global_Components/Base_AI_Character.Base_AI_Character_C|GetSpawn_Point (Variables|Default|GetWalking_AI_Character)) _newtrack_0) false false)))))

(event Custom|lunge%20forwards
  (bind _mesh (Variables|Character|GetMesh))
  (bind _walking_ai_character (Variables|Default|GetWalking_AI_Character))
  (bind _mesh_2 (Variables|Character|GetMesh))
  (bind _damageable (Variables|Default|GetDamageable))
  (bind _returnvalue (Components|SkeletalMesh|GetAnimInstance _mesh))
  (bind _returnvalue_2 (Components|SkeletalMesh|GetAnimInstance _mesh_2))
  (bind _aicharacter_state (Variables|/Game/SpyroContent/Global_Assets/Global_Components/Base_AI_Character.Base_AI_Character_C|GetAICharacter_State _walking_ai_character))
  (bind _returnvalue_3 (Utilities|Enum|Equal(Enum) _aicharacter_state "NewEnumerator2"))
  (CallFunction|EatingPing)
  (bind _askiller_bush_2_abp (Utilities|Casting|CastToKiller_Bush_2_ABP _returnvalue)
    (:then
      (if (not (Variables|/Game/MrTeaSpoonContent/StandaloneLevels/Enemies/Bush/Killer_Bush_2_ABP.Killer_Bush_2_ABP_C|GetisEating _askiller_bush_2_abp))
        (CallFunction|StopReturningHome :!label _label)
        (Utilities|FlowControl|Sequence
          (:then_0
            (bind _newtrack_0 (Timeline|Timeline_1 PlayFromStart)
              (:Update
                (if (and (not (Variables|/Game/SpyroContent/Global_Assets/Global_Components/Damageable_Com.Damageable_Com_C|GetFrozen _damageable)) (not (Variables|/Game/SpyroContent/Global_Assets/Global_Components/Damageable_Com.Damageable_Com_C|GetParalyzed_by_Fear _damageable)))
                  (Transformation|SetActorLocation (Math|Vector|Lerp(Vector) (Transformation|GetActorLocation) (+ (Variables|/Game/SpyroContent/Global_Assets/Global_Components/Base_AI_Character.Base_AI_Character_C|GetSpawn_Point (Variables|Default|GetWalking_AI_Character)) (* (Transformation|GetActorForwardVector) (Variables|Default|GetForward%20Travel%20Amount))) _newtrack_0) false false)))))
          (:then_1
            (Utilities|FlowControl|Delay 0.5)
            (bind _askiller_bush_2_abp_2 (Utilities|Casting|CastToKiller_Bush_2_ABP _returnvalue_2)
              (:then
                (if (and (not (Variables|/Game/MrTeaSpoonContent/StandaloneLevels/Enemies/Bush/Killer_Bush_2_ABP.Killer_Bush_2_ABP_C|GetisEating _askiller_bush_2_abp_2)) _returnvalue_3)
                  (CallFunction|ReturnHome :!label _label_2)
                  (Default|ChangeAICharacterState (Variables|Default|GetWalking_AI_Character) "NewEnumerator0")))
              (:CastFailed
                (bind _askiller_bush_3_abp (Utilities|Casting|CastToKiller_Bush_3_ABP _returnvalue_2))
                (if (and (not (Variables|/Game/MrTeaSpoonContent/StandaloneLevels/Enemies/Bush/Killer_Bush_3_ABP.Killer_Bush_3_ABP_C|GetisEating _askiller_bush_3_abp)) _returnvalue_3)
                  (goto _label_2))))))))
    (:CastFailed
      (bind _askiller_bush_3_abp_2 (Utilities|Casting|CastToKiller_Bush_3_ABP _returnvalue))
      (if (not (Variables|/Game/MrTeaSpoonContent/StandaloneLevels/Enemies/Bush/Killer_Bush_3_ABP.Killer_Bush_3_ABP_C|GetisEating _askiller_bush_3_abp_2))
        (goto _label)))))

(event Custom|Stop%20Lunging%20Forwards
  (bind _damageable (Variables|Default|GetDamageable))
  (bind _newtrack_0 (Timeline|Timeline_1 Stop)
    (:Update
      (if (and (not (Variables|/Game/SpyroContent/Global_Assets/Global_Components/Damageable_Com.Damageable_Com_C|GetFrozen _damageable)) (not (Variables|/Game/SpyroContent/Global_Assets/Global_Components/Damageable_Com.Damageable_Com_C|GetParalyzed_by_Fear _damageable)))
        (Transformation|SetActorLocation (Math|Vector|Lerp(Vector) (Transformation|GetActorLocation) (+ (Variables|/Game/SpyroContent/Global_Assets/Global_Components/Base_AI_Character.Base_AI_Character_C|GetSpawn_Point (Variables|Default|GetWalking_AI_Character)) (* (Transformation|GetActorForwardVector) (Variables|Default|GetForward%20Travel%20Amount))) _newtrack_0) false false)))))

(event EventBeginPlay
  (|CallParentFunction)
  (Components|DestroyComponent (Variables|Default|GetUnalert_Radius))
  (Variables|/Game/SpyroContent/Global_Assets/Global_Components/Damageable_Com.Damageable_Com_C|SetObject's%20Hitbox%20Component (Variables|Default|GetDamageable) (Variables|Default|GetBox_COL))
  (EventDispatchers|BindEventtoItemDropperSuccessfullyReset (Variables|Default|GetDrops_Items) (delegate Custom|On%20Bush%20Reset))
  (EventDispatchers|BindEventtoMyStateChanged (Variables|Default|GetWalking_AI_Character) (delegate Custom|Hedge%20State%20Changed)))

(fn ConstructionScript
  (|CallParentFunction))

(fn EatingPing
  (bind _eatingarea (Variables|Default|GetEatingArea))
  (bind _returnvalue (Transformation|GetWorldLocation _eatingarea))
  (bind _outhits (Class|KismetSystemLibrary|BoxTraceMultiforObjects _returnvalue _returnvalue (Variables|/Script/Engine.BoxComponent|GetBoxExtent _eatingarea) (Transformation|GetWorldRotation _eatingarea) (Utilities|Array|MakeArray "ObjectTypeQuery3" "ObjectTypeQuery9" "ObjectTypeQuery8" "ObjectTypeQuery10") false 0 "None" true))
  (bind _array_element (Utilities|Array|ForEachLoopwithBreak _outhits :!label _label)
    (:LoopBody
      (Utilities|Casting|CastToBP_Base_Playable (.hitactor _array_element))
      (bind _ate_a_player_ (CallFunction|CanIEatThisPlayer? (.hitactor _array_element) (.hitcomponent _array_element)))
      (if _ate_a_player_
        (goto _label Break)))))

(fn CanIEatThisPlayer?
  (params (other%20actor :type Object%20Object%20Reference) (other%20comp :type Object%20Object%20Reference))
  (bind _mesh (Variables|Character|GetMesh))
  (bind _damageable (Variables|Default|GetDamageable))
  (bind _returnvalue (Components|SkeletalMesh|GetAnimInstance _mesh))
  (Utilities|FlowControl|Sequence
    (:then_0
      (LocalVariables|Setate%20a%20player false)
      (bind _asbp_base_playable (Utilities|Casting|CastToBP_Base_Playable other%20actor))
      (if (Math|Boolean|ANDBoolean (== (Variables|/Script/Engine.Character|GetCapsuleComponent _asbp_base_playable) other%20comp) (not (Utilities|Enum|Equal(Enum) (Variables|/Game/SpyroContent/Global_Assets/Global_Characters/Playable_Characters/BP_Base_Playable.BP_Base_Playable_C|GetPlayer_State _asbp_base_playable) "NewEnumerator11")) (not (Variables|/Game/SpyroContent/Global_Assets/Global_Characters/Playable_Characters/BP_Base_Playable.BP_Base_Playable_C|GetRespawning _asbp_base_playable)) (Utilities|Enum|Equal(Enum) (Variables|/Game/SpyroContent/Global_Assets/Global_Components/Base_AI_Character.Base_AI_Character_C|GetAICharacter_State (Variables|Default|GetWalking_AI_Character)) "NewEnumerator2") (Utilities|Enum|Equal(Enum) (Variables|/Game/SpyroContent/Global_Assets/Global_Components/Damageable_Com.Damageable_Com_C|GetDamage_Being_Taken (Variables|/Game/SpyroContent/Global_Assets/Global_Characters/Playable_Characters/BP_Base_Playable.BP_Base_Playable_C|GetDamageable _asbp_base_playable)) "NewEnumerator6") (not (Variables|/Game/SpyroContent/Global_Assets/Global_Components/Damageable_Com.Damageable_Com_C|GetFrozen _damageable)) (not (Variables|/Game/SpyroContent/Global_Assets/Global_Components/Damageable_Com.Damageable_Com_C|GetParalyzed_by_Fear _damageable)))
        (bind _askiller_bush_2_abp (Utilities|Casting|CastToKiller_Bush_2_ABP _returnvalue)
          (:then
            (if (not (Variables|/Game/MrTeaSpoonContent/StandaloneLevels/Enemies/Bush/Killer_Bush_2_ABP.Killer_Bush_2_ABP_C|GetisEating _askiller_bush_2_abp))
              (Variables|/Game/MrTeaSpoonContent/StandaloneLevels/Enemies/Bush/Killer_Bush_2_ABP.Killer_Bush_2_ABP_C|SetisEating _askiller_bush_2_abp true)
              (LocalVariables|Setate%20a%20player true :!label _label)
              (CallFunction|StopLungingForwards)
              (CallFunction|DisableThisPlayer'sInputs _asbp_base_playable)
              (Variables|Default|SetPlayer%20in%20My%20Mouth _asbp_base_playable)
              (Rendering|SetActorHiddenInGame _asbp_base_playable true)
              (Variables|/Script/Engine.CameraComponent|SetFieldOfView (Variables|Default|GetCamera) (Variables|/Script/Engine.CameraComponent|GetFieldOfView (Variables|/Game/SpyroContent/Global_Assets/Global_Characters/Playable_Characters/BP_Base_Playable.BP_Base_Playable_C|GetFollowCamera _asbp_base_playable)))
              (Game|Player|SetViewTargetwithBlend (Variables|/Game/SpyroContent/Global_Assets/Global_Characters/Playable_Characters/BP_Base_Playable.BP_Base_Playable_C|GetSpyroContr_Ref _asbp_base_playable) self 1.0 "VTBlend_EaseIn" 1.0 false)
              (bind _asbp_spyro (Utilities|Casting|CastToBP_Spyro _asbp_base_playable))
              (bind _asdragon_breath_bp (Utilities|Casting|CastToDragon_Breath_BP (Variables|/Script/Engine.ChildActorComponent|GetChildActor (Variables|/Game/SpyroContent/Global_Assets/Global_Characters/Playable_Characters/Spyro/BP_Spyro.BP_Spyro_C|GetDragonBreath _asbp_spyro))))
              (Variables|/Game/SpyroContent/Global_Assets/Global_Level_Items/Dragon_Breath/Blueprints/Dragon_Breath_BP.Dragon_Breath_BP_C|SetInvoked%20Hide%20Fire%20Breath _asdragon_breath_bp true)))
          (:CastFailed
            (bind _askiller_bush_3_abp (Utilities|Casting|CastToKiller_Bush_3_ABP _returnvalue))
            (if (not (Variables|/Game/MrTeaSpoonContent/StandaloneLevels/Enemies/Bush/Killer_Bush_3_ABP.Killer_Bush_3_ABP_C|GetisEating _askiller_bush_3_abp))
              (Variables|/Game/MrTeaSpoonContent/StandaloneLevels/Enemies/Bush/Killer_Bush_3_ABP.Killer_Bush_3_ABP_C|SetisEating _askiller_bush_3_abp true)
              (goto _label))))))
    (:then_1
      (return (LocalVariables|Getate%20a%20player)))))

(fn ReleasethePlayerinMyMouth
  (bind _player_in_my_mouth (Variables|Default|GetPlayer%20in%20My%20Mouth)
    (:then
      (Default|InvokedResetCamera _player_in_my_mouth)
      (Game|Player|SetViewTargetwithBlend (Variables|/Game/SpyroContent/Global_Assets/Global_Characters/Playable_Characters/BP_Base_Playable.BP_Base_Playable_C|GetSpyroContr_Ref _player_in_my_mouth) _player_in_my_mouth 0.5 "VTBlend_Linear" 0.0 false)
      (Input|EnableInput _player_in_my_mouth (Variables|/Game/SpyroContent/Global_Assets/Global_Characters/Playable_Characters/BP_Base_Playable.BP_Base_Playable_C|GetSpyroContr_Ref _player_in_my_mouth))
      (Variables|/Game/SpyroContent/Global_Assets/Global_Characters/Playable_Characters/BP_Base_Playable.BP_Base_Playable_C|SetDid%20we%20disable%20input? _player_in_my_mouth false)
      (Rendering|SetActorHiddenInGame _player_in_my_mouth false)
      (bind _asbp_spyro (Utilities|Casting|CastToBP_Spyro _player_in_my_mouth)
        (:then
          (bind _asdragon_breath_bp (Utilities|Casting|CastToDragon_Breath_BP (Variables|/Script/Engine.ChildActorComponent|GetChildActor (Variables|/Game/SpyroContent/Global_Assets/Global_Characters/Playable_Characters/Spyro/BP_Spyro.BP_Spyro_C|GetDragonBreath _asbp_spyro)))
            (:then
              (Variables|/Game/SpyroContent/Global_Assets/Global_Level_Items/Dragon_Breath/Blueprints/Dragon_Breath_BP.Dragon_Breath_BP_C|SetInvoked%20Hide%20Fire%20Breath _asdragon_breath_bp false))
            (:CastFailed
              _)))
        (:CastFailed
          _))
      (Variables|Default|SetPlayer%20in%20My%20Mouth 0))
    (:else)))