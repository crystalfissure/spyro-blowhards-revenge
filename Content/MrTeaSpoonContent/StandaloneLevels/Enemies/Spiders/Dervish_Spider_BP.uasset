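; Spider enemy that charges the player and deals super damage through its eating hitbox while attacking, sparing a supercharging Spyro.
; AI state changes drive a delayed charge on Tick, optionally held back by off-camera mercy, with walk speed set by difficulty.
; When idle it returns to its spawn point or faces a nearby rival, feeding that rival's status to the AnimBP.
; Nest-spawned spiders self-destruct on poof or reset; poofing triggers nest respawns.
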(event OnComponentBeginOverlap(eating_hitbox)
  (params (OverlappedComponent :type Primitive%20Component%20Object%20Reference) (OtherActor :type Actor%20Object%20Reference) (OtherComp :type Primitive%20Component%20Object%20Reference) (OtherBodyIndex :type Integer) (bFromSweep :type Boolean) (SweepResult :type Hit%20Result%20Structure%20%28by%20ref%29))
  (bind _returnvalue (Actor|GetComponentbyClass OtherActor "/Game/SpyroContent/Global_Assets/Global_Components/Damageable_Com.Damageable_Com_C"))
  (Utilities|IsValid _returnvalue
    (:Is%20Valid
      (if (Utilities|Enum|Equal(Enum) (Variables|/Game/SpyroContent/Global_Assets/Global_Components/Base_AI_Character.Base_AI_Character_C|GetAICharacter_State (Variables|Default|GetWalking_AI_Character)) "NewEnumerator2")
        (bind _asbp_base_playable (Utilities|Casting|CastToBP_Base_Playable OtherActor)
          (:then
            (bind _asbp_spyro (Utilities|Casting|CastToBP_Spyro _asbp_base_playable)
              (:then
                (if (not (Variables|/Game/SpyroContent/Global_Assets/Global_Characters/Playable_Characters/Spyro/BP_Spyro.BP_Spyro_C|Getis_Currently_Supercharging _asbp_spyro))
                  (Default|DealDamage _returnvalue "NewEnumerator4" (Transformation|GetActorForwardVector) true self false :!label _label)))
              (:CastFailed
                (goto _label))))
          (:CastFailed
            (Utilities|Casting|CastToDervish_Spider_BP OtherActor
              (:then
                (if (Variables|Default|Getfriendly%20fire)
                  (goto _label)))
              (:CastFailed
                (Utilities|Casting|CastToStaticTree_BP OtherActor
                  (:CastFailed
                    (goto _label)))))))))))

(event Custom|On%20graboid%20State%20Changed
  (switch Utilities|FlowControl|Switch|SwitchonAICharacter_States (Variables|/Game/SpyroContent/Global_Assets/Global_Components/Base_AI_Character.Base_AI_Character_C|GetAICharacter_State (Variables|Default|GetWalking_AI_Character))
    (:NewEnumerator0
      (Variables|Default|SetRunning%20at%20player false :!label _label)
      (Variables|Default|Setmouth%20open false)
      (Audio|Components|Audio|Stop (Variables|Default|GetCharacter's%20Voice)))
    (:NewEnumerator1
      (Variables|Default|Setmouth%20open false)
      (CallFunction|RunatPlayer :!label _label_2))
    (:NewEnumerator2
      (goto _label_2))
    (:NewEnumerator3
      (goto _label))))

(event Custom|Run%20at%20Player
  (bind _walking_ai_character (Variables|Default|GetWalking_AI_Character))
  (bind _aicharacter_state (Variables|/Game/SpyroContent/Global_Assets/Global_Components/Base_AI_Character.Base_AI_Character_C|GetAICharacter_State _walking_ai_character))
  (Utilities|FlowControl|DoOnce false :!label _label
    (:Completed
      (Utilities|FlowControl|Delay 1.0)
      (if (or (Utilities|Enum|Equal(Enum) _aicharacter_state "NewEnumerator1") (Utilities|Enum|Equal(Enum) _aicharacter_state "NewEnumerator2"))
        (Variables|Default|SetRunning%20at%20player true)
        (goto _label Reset)
        (else
          (goto _label Reset))))))

(event Custom|Growth%20Spurt
  (Utilities|FlowControl|Delay 1.0)
  (bind _newtrack_0 (Timeline|Timeline_1 PlayFromStart)
    (:Update
      (if (not (Utilities|Enum|Equal(Enum) (Variables|/Game/SpyroContent/Global_Assets/Global_Components/Base_AI_Character.Base_AI_Character_C|GetAICharacter_State (Variables|Default|GetWalking_AI_Character)) "NewEnumerator3"))
        (Transformation|SetActorScale3D (Math|Vector|Lerp(Vector) "0.100000,0.100000,0.100000" "1.000000,1.000000,1.000000" _newtrack_0))))))

(event Custom|destroy%20self
  (Actor|DestroyActor))

(event Custom|on%20poof
  (bind _my_nest (Variables|Default|GetMy%20Nest)
    (:then
      (Default|SpawnDragoid _my_nest))
    (:else)))

(event Custom|clear%20dragoid%20corpse
  (if (Variables|Default|Getspawned%20from%20nest)
    (Utilities|FlowControl|Delay 0.2)
    (Actor|DestroyActor)))

(event EventSetMyDifficulty
  (bind _medium_walk_speed (Variables|Default|GetMedium%20Walk%20Speed))
  (bind _medium_walk_speed_2 (Variables|Default|GetMedium%20Walk%20Speed))
  (|CallParentFunction)
  (bind _asspyro_universal_save_data (CallFunction|LoadUniversalSave))
  (if (Utilities|Enum|Equal(Enum) (Variables|/Game/SpyroContent/Global_Assets/Global_SaveData/Spyro_Universal_Save_Data.Spyro_Universal_Save_Data_C|GetDifficulty _asspyro_universal_save_data) "NewEnumerator4")
    (bind _asspyro_save_data (CallFunction|LoadSpyroGame self))
    (bind _difficulty (CallFunction|ConvertSkillLevelFloattoEnum (Variables|/Game/SpyroContent/Global_Assets/Global_SaveData/Spyro_SaveData.Spyro_SaveData_C|GetSkill_Level _asspyro_save_data)))
    (Variables|/Script/Engine.CharacterMovementComponent|SetMaxWalkSpeed (Variables|Character|GetCharacterMovement) (Utilities|Select :Index _difficulty :NewEnumerator4 _medium_walk_speed :NewEnumerator0 (Variables|Default|GetEasy%20Walk%20Speed) :NewEnumerator1 _medium_walk_speed :NewEnumerator2 (Variables|Default|GetHard%20Walk%20Speed) :NewEnumerator3 (Variables|Default|GetNightmare%20Walk%20Speed)))
    (Variables|Default|SetDefault%20Walk%20Speed (Utilities|Select :Index _difficulty :NewEnumerator4 _medium_walk_speed :NewEnumerator0 (Variables|Default|GetEasy%20Walk%20Speed) :NewEnumerator1 _medium_walk_speed :NewEnumerator2 (Variables|Default|GetHard%20Walk%20Speed) :NewEnumerator3 (Variables|Default|GetNightmare%20Walk%20Speed)))
    (else
      (Variables|/Script/Engine.CharacterMovementComponent|SetMaxWalkSpeed (Variables|Character|GetCharacterMovement) (Utilities|Select :Index (Variables|/Game/SpyroContent/Global_Assets/Global_SaveData/Spyro_Universal_Save_Data.Spyro_Universal_Save_Data_C|GetDifficulty _asspyro_universal_save_data) :NewEnumerator4 _medium_walk_speed_2 :NewEnumerator0 (Variables|Default|GetEasy%20Walk%20Speed) :NewEnumerator1 _medium_walk_speed_2 :NewEnumerator2 (Variables|Default|GetHard%20Walk%20Speed) :NewEnumerator3 (Variables|Default|GetNightmare%20Walk%20Speed)))
      (Variables|Default|SetDefault%20Walk%20Speed (Utilities|Select :Index (Variables|/Game/SpyroContent/Global_Assets/Global_SaveData/Spyro_Universal_Save_Data.Spyro_Universal_Save_Data_C|GetDifficulty _asspyro_universal_save_data) :NewEnumerator4 _medium_walk_speed_2 :NewEnumerator0 (Variables|Default|GetEasy%20Walk%20Speed) :NewEnumerator1 _medium_walk_speed_2 :NewEnumerator2 (Variables|Default|GetHard%20Walk%20Speed) :NewEnumerator3 (Variables|Default|GetNightmare%20Walk%20Speed))))))

(event EventOnMovementModeChanged
  (params (PrevMovementMode :type EMovementMode%20Enum :default "MOVE_None") (NewMovementMode :type EMovementMode%20Enum :default "MOVE_None") (PrevCustomMode :type Byte :default 0) (NewCustomMode :type Byte :default 0))
  (|CallParentFunction PrevMovementMode NewMovementMode PrevCustomMode NewCustomMode)
  (if (and (Utilities|Enum|Equal(Enum) PrevMovementMode "MOVE_Falling") (Utilities|Enum|Equal(Enum) NewMovementMode "MOVE_Walking"))
    (Utilities|FlowControl|DoOnce false
      (:Completed
        (Variables|/Game/SpyroContent/Global_Assets/Global_Components/Base_AI_Character.Base_AI_Character_C|SetSpawn_Point (Variables|Default|GetWalking_AI_Character) (Transformation|GetActorLocation))))))

(event EventBeginPlay
  (bind _walking_ai_character (Variables|Default|GetWalking_AI_Character))
  (|CallParentFunction)
  (EventDispatchers|BindEventtoCorpsePoofed (Variables|Default|GetWalking_AI_Character) (delegate Custom|clear%20dragoid%20corpse))
  (EventDispatchers|BindEventtoMyStateChanged _walking_ai_character (delegate Custom|On%20graboid%20State%20Changed))
  (EventDispatchers|BindEventtoCorpsePoofed _walking_ai_character (delegate Custom|on%20poof))
  (bind _asspyro_persistant_data (Utilities|Casting|CastToSpyro_PersistantData (Game|GetGameInstance))
    (:then
      (EventDispatchers|BindEventtoUnloadLevel _asspyro_persistant_data (delegate Custom|destroy%20self)))
    (:CastFailed
      _))
  (Utilities|FlowControl|Delay (Variables|Default|Getanim%20delay))
  (bind _asdragoid_abp (Utilities|Casting|CastToDragoid_ABP (Components|SkeletalMesh|GetAnimInstance (Variables|Character|GetMesh))))
  (Variables|/Game/SpyroContent/CiC_Assets/CiC_Levels/Home_00_PastChasms/02_AridBasin/Actors/Dragoid/Dragoid_ABP.Dragoid_ABP_C|Setaggressive%20idle _asdragoid_abp (Variables|Default|Getaggressive%20idle))
  (Variables|Default|Getmy%20enemy
    (:then
      (Utilities|Time|SetTimerbyFunctionName 0 "enemy check" 1.0 true))
    (:else)))

(event EventTick
  (params (DeltaSeconds :type Float%20%28single-precision%29))
  (|CallParentFunction DeltaSeconds)
  (if (not (AI|Components|NavMovement|IsFalling (Variables|Character|GetCharacterMovement)))
    (if (Variables|Default|GetRunning%20at%20player)
      (bind _returnvalue (CallFunction|AmIonCamera?))
      (if (or (and _returnvalue (not (Variables|Default|GetDamaged%20Player,%20Show%20Mercy))) (not (Variables|Default|GetOff%20Camera%20Mercy)))
        (Pawn|Input|AddMovementInput (Transformation|GetActorForwardVector) 1.0 false))
      (else
        (switch Utilities|FlowControl|Switch|SwitchonAICharacter_States (Variables|/Game/SpyroContent/Global_Assets/Global_Components/Base_AI_Character.Base_AI_Character_C|GetAICharacter_State (Variables|Default|GetWalking_AI_Character))
          (:NewEnumerator0
            (if (> (Math|Float|Absolute(Float) (Math|Vector|VectorLength (- (Variables|/Game/SpyroContent/Global_Assets/Global_Components/Base_AI_Character.Base_AI_Character_C|GetSpawn_Point (Variables|Default|GetWalking_AI_Character)) (Transformation|GetActorLocation)))) 1.5e+02)
              (Transformation|SetActorRotation (Math|Rotator|Lerp(Rotator) (Transformation|GetActorRotation) (Math|Rotator|MakeRotator 0.0 0.0 (.yaw (Math|Rotator|FindLookatRotation (Transformation|GetActorLocation) (Variables|/Game/SpyroContent/Global_Assets/Global_Components/Base_AI_Character.Base_AI_Character_C|GetSpawn_Point (Variables|Default|GetWalking_AI_Character))))) (* (Utilities|Time|GetWorldDeltaSeconds) 2e+01) true))
              (Pawn|Input|AddMovementInput (Transformation|GetActorForwardVector) 1.0 false)
              (else
                (bind _my_enemy (Variables|Default|Getmy%20enemy)
                  (:then
                    (if (and (not (Utilities|Enum|Equal(Enum) (Variables|/Game/SpyroContent/Global_Assets/Global_Components/Base_AI_Character.Base_AI_Character_C|GetAICharacter_State (Variables|/Game/SpyroContent/Global_Assets/Global_Characters/AI_Characters/Actors/Base_AICharacter_BP.Base_AICharacter_BP_C|GetWalking_AI_Character _my_enemy)) "NewEnumerator3")) (<= (Transformation|GetDistanceTo self) 5.5e+02))
                      (Transformation|SetActorRotation (Math|Rotator|Lerp(Rotator) (Transformation|GetActorRotation) (Math|Rotator|MakeRotator 0.0 0.0 (.yaw (Math|Rotator|FindLookatRotation (Transformation|GetActorLocation) (Transformation|GetActorLocation (Variables|Default|Getmy%20enemy))))) (* (Utilities|Time|GetWorldDeltaSeconds) 2e+01) true))))
                  (:else))))))))))

(event EventResetThisAICharacter
  (|CallParentFunction)
  (Variables|Default|SetRunning%20at%20player false)
  (if (Variables|Default|Getspawned%20from%20nest)
    (Actor|DestroyActor)))

(fn ConstructionScript
  (|CallParentFunction))

(fn EnemyCheck
  (bind _my_enemy (Variables|Default|Getmy%20enemy)
    (:then
      (bind _asdragoid_abp (Utilities|Casting|CastToDragoid_ABP (Components|SkeletalMesh|GetAnimInstance (Variables|Character|GetMesh))))
      (Variables|/Game/SpyroContent/CiC_Assets/CiC_Levels/Home_00_PastChasms/02_AridBasin/Actors/Dragoid/Dragoid_ABP.Dragoid_ABP_C|Setmy%20enemy%20is%20dead _asdragoid_abp (or (Utilities|Enum|Equal(Enum) (Variables|/Game/SpyroContent/Global_Assets/Global_Components/Base_AI_Character.Base_AI_Character_C|GetAICharacter_State (Variables|/Game/SpyroContent/Global_Assets/Global_Characters/AI_Characters/Actors/Base_AICharacter_BP.Base_AICharacter_BP_C|GetWalking_AI_Character _my_enemy)) "NewEnumerator3") (> (Transformation|GetDistanceTo _my_enemy self) 5.5e+02))))
    (:else)))