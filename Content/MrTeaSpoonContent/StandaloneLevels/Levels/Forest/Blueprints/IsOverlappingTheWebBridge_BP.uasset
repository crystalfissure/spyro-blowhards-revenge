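; Forest level trigger for the web bridge that drowns Spyro whenever he is on it without supercharging.
; The static mesh's begin and end overlaps, filtered to a playable's capsule component, set an overlap flag and cache the player, actor and component.
; While the flag is set, Tick checks Spyro's supercharge state and, if he is not supercharging, calls DrownThePlayer on the referenced drownable web.
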(event OnComponentBeginOverlap(StaticMesh)
  (params (OverlappedComponent :type Primitive%20Component%20Object%20Reference) (OtherActor :type Actor%20Object%20Reference) (OtherComp :type Primitive%20Component%20Object%20Reference) (OtherBodyIndex :type Integer) (bFromSweep :type Boolean) (SweepResult :type Hit%20Result%20Structure%20%28by%20ref%29))
  (bind _asbp_base_playable (Utilities|Casting|CastToBP_Base_Playable OtherActor))
  (if (== (Variables|/Script/Engine.Character|GetCapsuleComponent _asbp_base_playable) OtherComp)
    (Variables|Default|SetisOverlappingTheBridge true)
    (Variables|Default|SetBP%20Base%20Playable%20Ref _asbp_base_playable)
    (Variables|Default|SetOther%20Actor OtherActor)
    (Variables|Default|SetOther%20Comp OtherComp)))

(event OnComponentEndOverlap(StaticMesh)
  (params (OverlappedComponent :type Primitive%20Component%20Object%20Reference) (OtherActor :type Actor%20Object%20Reference) (OtherComp :type Primitive%20Component%20Object%20Reference) (OtherBodyIndex :type Integer))
  (bind _asbp_base_playable (Utilities|Casting|CastToBP_Base_Playable OtherActor))
  (if (== (Variables|/Script/Engine.Character|GetCapsuleComponent _asbp_base_playable) OtherComp)
    (Variables|Default|SetisOverlappingTheBridge false)))

(event EventTick
  (params (DeltaSeconds :type Float%20%28single-precision%29))
  (if (Variables|Default|GetisOverlappingTheBridge)
    (bind _asbp_spyro (Utilities|Casting|CastToBP_Spyro (Variables|Default|GetBP%20Base%20Playable%20Ref)))
    (if (not (Variables|/Game/SpyroContent/Global_Assets/Global_Characters/Playable_Characters/Spyro/BP_Spyro.BP_Spyro_C|Getis_Currently_Supercharging _asbp_spyro))
      (Default|DrownthePlayer (Variables|Default|GetDrownable%20Web%20Ref) (Variables|Default|GetOther%20Actor) (Variables|Default|GetOther%20Comp)))))

(fn ConstructionScript)