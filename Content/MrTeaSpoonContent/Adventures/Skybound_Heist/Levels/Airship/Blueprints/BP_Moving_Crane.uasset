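; BP_Moving_Crane is an ambient crane in the Skybound Heist airship level that slides its static mesh back and forth along its local X axis.
; After a random delay, MoveAgain picks a random target offset, mirrored negative for right-side cranes via RightCrane, and sets the travel direction.
; Tick steps the mesh by a fixed MoveSpeed per frame, not scaled by delta time, until near the target, then triggers MoveAgain again.
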(event Custom|Move%20again
  (bind _returnvalue (Math|Random|RandomFloatinRange 0.0 1.5e+03))
  (Utilities|FlowControl|Delay (Math|Random|RandomFloatinRange 7.0 19.0))
  (Variables|Default|SetMove%20to%20target (select (Variables|Default|GetRight%20crane) (* _returnvalue -1.0) _returnvalue))
  (Variables|Default|SetArrived%20at%20target false)
  (if (<= (Variables|Default|GetMove%20to%20target) (.X (Math|Vector|BreakVector (.Location (Math|Transform|BreakTransform (Transformation|GetRelativeTransform (Variables|Default|GetStaticMesh)))))))
    (Variables|Default|SetMoving%20backwards true)
    (else
      (Variables|Default|SetMoving%20backwards false))))

(event EventBeginPlay
  (bind _returnvalue (Math|Random|RandomFloatinRange 0.0 1.5e+03))
  (Utilities|FlowControl|Delay (Math|Random|RandomFloatinRange 7.0 19.0))
  (Variables|Default|SetMove%20to%20target (select (Variables|Default|GetRight%20crane) (* _returnvalue -1.0) _returnvalue))
  (Variables|Default|SetArrived%20at%20target false)
  (if (<= (Variables|Default|GetMove%20to%20target) (.X (Math|Vector|BreakVector (.Location (Math|Transform|BreakTransform (Transformation|GetRelativeTransform (Variables|Default|GetStaticMesh)))))))
    (Variables|Default|SetMoving%20backwards true)
    (else
      (Variables|Default|SetMoving%20backwards false))))

(event EventTick
  (params (DeltaSeconds :type Float%20%28single-precision%29))
  (bind _move_speed (Variables|Default|GetMove%20speed))
  (bind _staticmesh (Variables|Default|GetStaticMesh))
  (bind _returnvalue (Transformation|GetRelativeTransform _staticmesh))
  (bind _location (Math|Transform|BreakTransform _returnvalue))
  (bind _x (Math|Vector|BreakVector _location))
  (if (not (Variables|Default|GetArrived%20at%20target))
    (if (Math|Float|NearlyEqual(Float) (Variables|Default|GetMove%20to%20target) _x 1e+01)
      (Variables|Default|SetArrived%20at%20target true)
      (CallFunction|MoveAgain)
      (else
        (Transformation|SetRelativeLocation (Variables|Default|GetStaticMesh) (Math|Vector|MakeVector (select (Variables|Default|GetMoving%20backwards) (- _x _move_speed) (+ _x _move_speed)) 0.0 0.0) false false)))))

(fn ConstructionScript)