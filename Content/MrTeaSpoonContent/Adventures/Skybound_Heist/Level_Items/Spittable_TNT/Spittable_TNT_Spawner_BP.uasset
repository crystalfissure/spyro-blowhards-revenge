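; Spawner actor that ejects a spittable TNT object in the Skybound Heist adventure.
; Its SpawnLavaRock event spawns the TNT at a forward offset, sets its state, enables physics and launches it up and forward with a velocity-change impulse.
; It registers itself as the TNT's spawner and plays a lava rock spit sound.
; Nothing in this Blueprint calls the event, and its default events are disabled.
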(event EventBeginPlay
  (|CallParentFunction) ; This node is disabled and will not be called.\nDrag off pins to build functionality.
)

(event Collision|EventActorBeginOverlap
  (params (OtherActor :type Actor%20Object%20Reference))
  (|CallParentFunction OtherActor) ; This node is disabled and will not be called.\nDrag off pins to build functionality.
)

(event EventTick
  (params (DeltaSeconds :type Float%20%28single-precision%29))
  (|CallParentFunction DeltaSeconds) ; This node is disabled and will not be called.\nDrag off pins to build functionality.
)

(event EventSpawnLavaRock
  (bind _returnvalue (Game|SpawnActorfromClass "/Game/MrTeaSpoonContent/Adventures/Skybound_Heist/Level_Items/Spittable_TNT/Spittable_TNT_BP.Spittable_TNT_BP_C" (Math|Transform|MakeTransform (+ (.location (Transformation|GetActorTransform)) (* (Transformation|GetActorForwardVector) (Variables|Default|Getforward%20offset))) "0, 0, 0" "1,1,1") "AdjustIfPossibleButAlwaysSpawn" 0 0))
  (Variables|/Game/SpyroContent/Global_Assets/Global_Level_Items/Spittable_Object/Base_Spittable_Object_BP.Base_Spittable_Object_BP_C|SetSpittable%20Object%20State _returnvalue "NewEnumerator1")
  (Physics|SetSimulatePhysics (Variables|/Game/SpyroContent/Global_Assets/Global_Level_Items/Spittable_Object/Base_Spittable_Object_BP.Base_Spittable_Object_BP_C|GetCOL _returnvalue) true)
  (Physics|AddImpulse (Variables|/Game/SpyroContent/Global_Assets/Global_Level_Items/Spittable_Object/Base_Spittable_Object_BP.Base_Spittable_Object_BP_C|GetCOL _returnvalue) (+ (* (Transformation|GetActorUpVector) 5e+02) (* (Transformation|GetActorForwardVector) 2.5e+02)) "None" true)
  (Variables|/Game/SpyroContent/Global_Assets/Global_Level_Items/Spittable_Object/LavaRock/LavaRock_BP.LavaRock_BP_C|SetMy%20Spawner _returnvalue self)
  (Audio|PlaySoundatLocation "/Game/SpyroContent/Global_Assets/Global_Level_Items/Spittable_Object/LavaRock/lava_rock_spit.lava_rock_spit" (Transformation|GetActorLocation) "0, 0, 0" 1.0 1.0 0.0 0 0 0))

(fn ConstructionScript
  (|CallParentFunction))