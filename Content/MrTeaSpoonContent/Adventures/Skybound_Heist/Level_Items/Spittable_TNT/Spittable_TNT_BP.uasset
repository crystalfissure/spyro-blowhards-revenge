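; Spittable TNT item for the Skybound Heist adventure level.
; When the actor is destroyed, it plays an explosion sound with attenuation at its location and spawns a Superflame blast particle emitter there.
; The graph holds no other active logic, as BeginPlay, Tick and overlap events are disabled and the construction script only calls its parent.
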(event EventBeginPlay
  (|CallParentFunction) ; This node is disabled and will not be called.\nDrag off pins to build functionality.
)

(event Collision|EventActorBeginOverlap
  (params (OtherActor :type Actor%20Object%20Reference))
  (|CallParentFunction OtherActor) ; This node is disabled and will not be called.\nDrag off pins to build functionality.
)

(event EventTick
  (params (DeltaSeconds :type Float%20%28single-precision%29))
  (|CallParentFunction DeltaSeconds) ; This node is disabled and will not be called.\nDrag off pins to build functionality.
)

(event EventDestroyed
  (Audio|PlaySoundatLocation "/Game/MrTeaSpoonContent/Adventures/Skybound_Heist/Level_Items/Spittable_TNT/Assets/SFX_TNTExplode.SFX_TNTExplode" (Transformation|GetActorLocation) "0, 0, 0" 1.0 1.0 0.0 "/Game/SpyroContent/Global_Assets/Global_Audio/Attenuation/Spyro_Attenuation_Farther.Spyro_Attenuation_Farther" 0 0)
  (Effects|SpawnEmitteratLocation "/Game/SpyroContent/Global_Assets/Global_Level_Items/Superflame/Particles/Superflame_Blast.Superflame_Blast" (Transformation|GetActorLocation)))

(fn ConstructionScript
  (|CallParentFunction))