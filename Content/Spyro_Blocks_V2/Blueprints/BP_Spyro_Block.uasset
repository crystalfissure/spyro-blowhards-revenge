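; BP_Spyro_Block is a placeable block actor with a selectable shape and tile index.
; The construction script assigns the chosen BlockShape to the static mesh and writes ChosenTileIndex into a custom primitive data slot.
; BeginPlay writes the same index again at runtime.
; Custom primitive data exposes the tile choice per block to materials without needing dynamic material instances.
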(event EventBeginPlay
  (Rendering|Material|SetCustomPrimitiveDataFloat (Variables|Default|GetStaticMesh) 12 (Math|Conversions|ToFloat(Integer) (Variables|Default|GetChosen%20Tile%20Index))))

(event Collision|EventActorBeginOverlap
  (params (OtherActor :type Actor%20Object%20Reference)))

(event EventTick
  (params (DeltaSeconds :type Float%20%28single-precision%29)))

(fn ConstructionScript
  (Components|StaticMesh|SetStaticMesh (Variables|Default|GetStaticMesh) (Variables|Default|GetBlock%20Shape))
  (Rendering|Material|SetCustomPrimitiveDataFloat (Variables|Default|GetStaticMesh) 12 (Math|Conversions|ToFloat(Integer) (Variables|Default|GetChosen%20Tile%20Index))))