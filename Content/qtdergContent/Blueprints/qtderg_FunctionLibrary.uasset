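; Blueprint function library with an overlap filter for the playable character and a save-data query.
; BasePlayableOverlapped casts the other actor to BP_Base_Playable and reports whether the overlapped component is its capsule.
; NewFunction_0 loads the Spyro save and checks one hard-indexed item-collected flag in the level item info.
; That check looks unfinished, as it only ever assigns false to the local variable it returns.
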(fn BasePlayableOverlapped
  (params (Other%20Actor :type Actor%20Object%20Reference) (Other%20Comp :type Primitive%20Component%20Object%20Reference))
  (bind _asbp_base_playable (Utilities|Casting|CastToBP_Base_Playable Other%20Actor))
  (return (== (Variables|/Script/Engine.Character|GetCapsuleComponent _asbp_base_playable) Other%20Comp)))

(fn NewFunction0
  (bind _self self)
  (bind _asspyro_save_data (CallFunction|LoadSpyroGame _self 0 _self))
  (if (Utilities|Array|Get(acopy) (.itemsplayergot (Utilities|Array|Get(acopy) (.membervar_0 (Utilities|Array|Get(acopy) (Variables|/Game/SpyroContent/Global_Assets/Global_SaveData/Spyro_SaveData.Spyro_SaveData_C|GetLevel_Item_Info _asspyro_save_data))) 1)))
    _
    (else
      (LocalVariables|SetNewLocalVar_0 false)))
  (return (LocalVariables|GetNewLocalVar_0)))