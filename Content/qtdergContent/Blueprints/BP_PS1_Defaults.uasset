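; BP_PS1_Defaults applies PS1-style graphics defaults to the Universal Save the first time it runs for its save slot.
; On BeginPlay it checks a PS1_Defaults_SaveObject flag, proceeding if the save is missing or unflagged.
; It enables warble, distance fade, constrained aspect, pixelation and low-res font, with dithering set by a variable.
; It then saves, reloads options, triggers the font resolution update through Spyro_PersistantData and writes the flag.
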(event EventBeginPlay
  (bind _returnvalue (SaveGame|LoadGamefromSlot (Variables|Default|GetSave%20Slot%20Name)))
  (bind _asps1_defaults_save_object (Utilities|Casting|CastToPS1_Defaults_SaveObject _returnvalue)
    (:then
      (if (not (Variables|/Game/qtdergContent/Blueprints/PS1_Defaults_SaveObject.PS1_Defaults_SaveObject_C|GetDefaults%20have%20been%20set _asps1_defaults_save_object))
        (bind _asspyro_universal_save_data (CallFunction|LoadUniversalSave :!label _label))
        (Variables|/Game/SpyroContent/Global_Assets/Global_SaveData/Spyro_Universal_Save_Data.Spyro_Universal_Save_Data_C|SetPS1_Warble_Enabled _asspyro_universal_save_data true)
        (Variables|/Game/SpyroContent/Global_Assets/Global_SaveData/Spyro_Universal_Save_Data.Spyro_Universal_Save_Data_C|SetDistanceFade_Enabled _asspyro_universal_save_data true)
        (Variables|/Game/SpyroContent/Global_Assets/Global_SaveData/Spyro_Universal_Save_Data.Spyro_Universal_Save_Data_C|SetConstrainAspect _asspyro_universal_save_data true)
        (Variables|/Game/SpyroContent/Global_Assets/Global_SaveData/Spyro_Universal_Save_Data.Spyro_Universal_Save_Data_C|SetPixelation _asspyro_universal_save_data true)
        (Variables|/Game/SpyroContent/Global_Assets/Global_SaveData/Spyro_Universal_Save_Data.Spyro_Universal_Save_Data_C|SetDithering_Enabled _asspyro_universal_save_data (Variables|Default|GetDithering%20Enabled))
        (Variables|/Game/SpyroContent/Global_Assets/Global_SaveData/Spyro_Universal_Save_Data.Spyro_Universal_Save_Data_C|SetLow%20Res%20Font _asspyro_universal_save_data true)
        (SaveGame|SaveGametoSlot _asspyro_universal_save_data "Universal Save")
        (CallFunction|LoadUniversalSavedOptions self)
        (bind _asspyro_persistant_data (Utilities|Casting|CastToSpyro_PersistantData (Game|GetGameInstance)))
        (Default|CallFontResolutionChanged _asspyro_persistant_data)
        (bind _returnvalue_2 (SaveGame|CreateSaveGameObject "/Game/qtdergContent/Blueprints/PS1_Defaults_SaveObject.PS1_Defaults_SaveObject_C"))
        (Variables|/Game/qtdergContent/Blueprints/PS1_Defaults_SaveObject.PS1_Defaults_SaveObject_C|SetDefaults%20have%20been%20set _returnvalue_2 true)
        (SaveGame|SaveGametoSlot _returnvalue_2 (Variables|Default|GetSave%20Slot%20Name))))
    (:CastFailed
      (goto _label))))

(fn ConstructionScript)