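; Italian fairy Blueprint that recolors one material slot of its mesh when play begins.
; After the parent BeginPlay, it sets slot 12 to a vertex-color material, then replaces it with a dynamic instance of the two-sided variant.
; That instance receives a dark green color and a raised brightness through material parameters.
; The construction script only calls the parent, and Tick and overlap events are disabled.
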(event EventBeginPlay
  (bind _mesh (Variables|Character|GetMesh))
  (|CallParentFunction)
  (Rendering|Material|SetMaterial _mesh 12 "/Game/SpyroContent/Global_Assets/Global_Materials/Material_Instances/Untex_Vertex_Color.Untex_Vertex_Color")
  (bind _returnvalue (Rendering|Material|CreateDynamicMaterialInstance _mesh 12 "/Game/SpyroContent/Global_Assets/Global_Materials/Material_Instances/Untex_Vertex_Color_2Sided.Untex_Vertex_Color_2Sided" "None" :!class /Script/Engine.PrimitiveComponent))
  (Rendering|Material|SetVectorParameterValue _returnvalue "ColorChange" "(R=0.000000,G=0.266356,B=0.057805,A=1.000000)" :!class /Script/Engine.MaterialInstanceDynamic)
  (Rendering|Material|SetScalarParameterValue _returnvalue "Brightness" 3.0 :!class /Script/Engine.MaterialInstanceDynamic))

(event Collision|EventActorBeginOverlap
  (params (OtherActor :type Actor%20Object%20Reference))
  (|CallParentFunction OtherActor) ; This node is disabled and will not be called.\nDrag off pins to build functionality.
)

(event EventTick
  (params (DeltaSeconds :type Float%20%28single-precision%29))
  (|CallParentFunction DeltaSeconds) ; This node is disabled and will not be called.\nDrag off pins to build functionality.
)

(fn ConstructionScript
  (|CallParentFunction))