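; Debug checker actor that finds which treasure containers and enemies in the level have a blue butterfly among their item drops.
; Two seconds after BeginPlay, it gathers all treasure container and base enemy actors and loops through each one's ItemsToDrop list.
; Each entry that casts to Blue_Butterfly_BP prints the display name of its owning container or enemy to the screen.
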(event EventBeginPlay
  (Utilities|FlowControl|Delay 2.0)
  (bind _outactors (Actor|GetAllActorsOfClass "/Game/SpyroContent/Global_Assets/Global_Level_Items/Treasure_Containers/Treasure_Container_Base_BP.Treasure_Container_Base_BP_C"))
  (for _array_element _outactors
    (for _array_element_2 (Variables|/Game/SpyroContent/Global_Assets/Global_Components/Drops_Items.Drops_Items_C|GetItems_to_Drop (Variables|/Game/SpyroContent/Global_Assets/Global_Level_Items/Treasure_Containers/Treasure_Container_Base_BP.Treasure_Container_Base_BP_C|GetItem_Drop_Component _array_element))
      (Utilities|Casting|CastToBlue_Butterfly_BPClass _array_element_2)
      (Development|PrintString (Utilities|GetDisplayName _array_element))))
  (bind _outactors_2 (Actor|GetAllActorsOfClass "/Game/SpyroContent/Global_Assets/Global_Characters/AI_Characters/Actors/Enemies/Base_Enemy_BP.Base_Enemy_BP_C"))
  (for _array_element_3 _outactors_2
    (for _array_element_4 (Variables|/Game/SpyroContent/Global_Assets/Global_Components/Drops_Items.Drops_Items_C|GetItems_to_Drop (Variables|/Game/SpyroContent/Global_Assets/Global_Characters/AI_Characters/Actors/Base_AICharacter_BP.Base_AICharacter_BP_C|GetDrops_Items _array_element_3))
      (Utilities|Casting|CastToBlue_Butterfly_BPClass _array_element_4)
      (Development|PrintString (Utilities|GetDisplayName _array_element_3)))))

(fn ConstructionScript)