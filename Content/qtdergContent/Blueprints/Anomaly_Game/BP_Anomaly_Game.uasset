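; BP_Anomaly_Game runs a spot-the-anomaly floor game where players answer through Yes or No portals.
; Correct answers raise the gold floor number and wrong ones reset it, or drop one in easy mode; reaching MaxFloor teleports players to EndPoint.
; Otherwise they respawn, objects reset, and a coin flip may reveal the next shuffled anomaly, optionally hiding its normal counterpart.
; A DoOnce with delayed reset debounces portal overlaps.
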(event OnComponentBeginOverlap(Noanomaly)
  (params (OverlappedComponent :type Primitive%20Component%20Object%20Reference) (OtherActor :type Actor%20Object%20Reference) (OtherComp :type Primitive%20Component%20Object%20Reference) (OtherBodyIndex :type Integer) (bFromSweep :type Boolean) (SweepResult :type Hit%20Result%20Structure%20%28by%20ref%29))
  (CallFunction|PlayerWentThroughPortal OtherActor OtherComp false))

(event OnComponentBeginOverlap(Yesanomaly)
  (params (OverlappedComponent :type Primitive%20Component%20Object%20Reference) (OtherActor :type Actor%20Object%20Reference) (OtherComp :type Primitive%20Component%20Object%20Reference) (OtherBodyIndex :type Integer) (bFromSweep :type Boolean) (SweepResult :type Hit%20Result%20Structure%20%28by%20ref%29))
  (CallFunction|PlayerWentThroughPortal OtherActor OtherComp true))

(event Custom|Player%20went%20through%20portal
  (params (Other%20Actor :type Actor%20Object%20Reference) (Other%20Comp :type Primitive%20Component%20Object%20Reference) (Player%20believes%20there's%20an%20anomaly :type Boolean))
  (bind _asbp_base_playable (Utilities|Casting|CastToBP_Base_Playable Other%20Actor))
  (if (== (Variables|/Script/Engine.Character|GetCapsuleComponent _asbp_base_playable) Other%20Comp)
    (Utilities|FlowControl|DoOnce false
      (:Completed
        (if (not (Variables|Default|GetPlayer%20won%20the%20game))
          (if (Math|Boolean|Equal(Boolean) (Variables|Default|GetCurrent%20floor%20is%20an%20anomaly) Player%20believes%20there's%20an%20anomaly)
            (CallFunction|SUCCESS _asbp_base_playable)
            (else
              (CallFunction|FAIL _asbp_base_playable))))))))

(event Custom|SUCCESS
  (params (BP%20Base%20Playable%20Ref :type BP%20Base%20Playable%20Object%20Reference))
  (bind _respawn_point (Variables|Default|GetRespawn%20Point))
  (bind _returnvalue (Transformation|GetWorldTransform _respawn_point))
  (Math|Integer|IncrementInt (Variables|Default|GetCurrent%20floor)
    (:%20%20
      (CallFunction|SetGoldText)
      (Transformation|SetActorLocationAndRotation BP%20Base%20Playable%20Ref (.location _returnvalue) (.rotation _returnvalue))
      (CallFunction|ResetObjectstoDefaultState))))

(event Custom|FAIL
  (params (BP%20Base%20Playable%20Ref :type BP%20Base%20Playable%20Object%20Reference))
  (bind _respawn_point (Variables|Default|GetRespawn%20Point))
  (bind _returnvalue (Transformation|GetWorldTransform _respawn_point))
  (if (Variables|Default|GetEasy%20mode)
    (Variables|Default|SetCurrent%20floor (- (Variables|Default|GetCurrent%20floor) 1))
    (if (< (Variables|Default|GetCurrent%20floor) 0)
      (Variables|Default|SetCurrent%20floor 0))
    (else
      (Variables|Default|SetCurrent%20floor 0)))
  (CallFunction|SetGoldText)
  (Transformation|SetActorLocationAndRotation BP%20Base%20Playable%20Ref (.location _returnvalue) (.rotation _returnvalue))
  (CallFunction|ResetObjectstoDefaultState))

(event Custom|Reset
  (Utilities|FlowControl|Delay 1.0)
  (Utilities|FlowControl|DoOnce false) ; enters at Reset
)

(event Custom|Set%20gold%20text
  (Components|StaticMesh|SetStaticMesh (Variables|Default|GetCurrent%20Floor%20Text%20Gold) (Utilities|Select :Index (Variables|Default|GetCurrent%20floor) :Option%200 "/Game/SpyroContent/Global_Assets/Global_Level_Items/Golden_Text/static_meshes/gold_letters_all_Number_0.gold_letters_all_Number_0" :Option%201 "/Game/SpyroContent/Global_Assets/Global_Level_Items/Golden_Text/static_meshes/gold_letters_all_Number_1.gold_letters_all_Number_1" :Option%202 "/Game/SpyroContent/Global_Assets/Global_Level_Items/Golden_Text/static_meshes/gold_letters_all_Number_2.gold_letters_all_Number_2" :Option%203 "/Game/SpyroContent/Global_Assets/Global_Level_Items/Golden_Text/static_meshes/gold_letters_all_Number_3.gold_letters_all_Number_3" :Option%204 "/Game/SpyroContent/Global_Assets/Global_Level_Items/Golden_Text/static_meshes/gold_letters_all_Number_4.gold_letters_all_Number_4" :Option%205 "/Game/SpyroContent/Global_Assets/Global_Level_Items/Golden_Text/static_meshes/gold_letters_all_Number_5.gold_letters_all_Number_5" :Option%206 "/Game/SpyroContent/Global_Assets/Global_Level_Items/Golden_Text/static_meshes/gold_letters_all_Number_6.gold_letters_all_Number_6" :Option%207 "/Game/SpyroContent/Global_Assets/Global_Level_Items/Golden_Text/static_meshes/gold_letters_all_Number_7.gold_letters_all_Number_7" :Option%208 "/Game/SpyroContent/Global_Assets/Global_Level_Items/Golden_Text/static_meshes/gold_letters_all_Number_8.gold_letters_all_Number_8" :Option%209 "/Game/SpyroContent/Global_Assets/Global_Level_Items/Golden_Text/static_meshes/gold_letters_all_Number_9.gold_letters_all_Number_9")))

(event Custom|Reset%20objects%20to%20default%20state
  ;[0 0 0] This resets all the objects to their default state:
  ; Normal - visible and with collision
  ; Anomaly - hidden, collision disabled
  (for _array_element (Variables|Default|GetAnomaly%20Struct%20Array)
    (if (.Swap (Utilities|Struct|BreakAnomaly_Struct _array_element))
      (Rendering|SetActorHiddenInGame (.NormalObject (Utilities|Struct|BreakAnomaly_Struct _array_element)) false)
      (Collision|SetActorEnableCollision (.NormalObject (Utilities|Struct|BreakAnomaly_Struct _array_element)) true))
    (Rendering|SetActorHiddenInGame (.AnomalyObject (Utilities|Struct|BreakAnomaly_Struct _array_element)) true)
    (Collision|SetActorEnableCollision (.AnomalyObject (Utilities|Struct|BreakAnomaly_Struct _array_element)) false))
  (CallFunction|SpawnAnomaly))

(event Custom|Spawn%20anomaly
  (bind _end_point (Variables|Default|GetEnd%20Point))
  (bind _returnvalue (Transformation|GetWorldTransform _end_point))
  ;[0 0 0] Check if the current floor is the last
  ; True - end the game
  ; False - spawn the anomaly
  (if (== (Variables|Default|GetMax%20floor) (Variables|Default|GetCurrent%20floor))
    (Variables|Default|SetPlayer%20won%20the%20game true)
    (bind _returnvalue_2 (Actor|GetActorOfClass "/Game/SpyroContent/Global_Assets/Global_Characters/Playable_Characters/BP_Base_Playable.BP_Base_Playable_C"))
    (Transformation|SetActorLocationAndRotation _returnvalue_2 (.location _returnvalue) (.rotation _returnvalue))
    (else
      ;[0 0 0] 50/50 chance to spawn an anomaly
      (if (Math|Random|RandomBool)
        (Variables|Default|SetCurrent%20floor%20is%20an%20anomaly true)
        ;[0 0 0 1 16] Failsafe - if the array is exhausted due to player sucking at the game, the index is set to 0 and array is shuffled
        (Utilities|IsValid (.AnomalyObject (Utilities|Struct|BreakAnomaly_Struct (Utilities|Array|Get(acopy) (Variables|Default|GetAnomaly%20Struct%20Array) (Variables|Default|GetAnomaly%20index))))
          (:Is%20Valid
            _)
          (:Is%20Not%20Valid
            (Variables|Default|SetAnomaly%20index 0)
            (Utilities|Array|Shuffle (Variables|Default|GetAnomaly%20Struct%20Array))))
        ;[0 0 0] Check if it's a "swap" type anomaly
        ; If true, then the "Normal Object" needs to be hidden
        (if (.Swap (Utilities|Struct|BreakAnomaly_Struct (Utilities|Array|Get(acopy) (Variables|Default|GetAnomaly%20Struct%20Array) (Variables|Default|GetAnomaly%20index))))
          (Rendering|SetActorHiddenInGame (.NormalObject (Utilities|Struct|BreakAnomaly_Struct (Utilities|Array|Get(acopy) (Variables|Default|GetAnomaly%20Struct%20Array) (Variables|Default|GetAnomaly%20index)))) true)
          (Collision|SetActorEnableCollision (.NormalObject (Utilities|Struct|BreakAnomaly_Struct (Utilities|Array|Get(acopy) (Variables|Default|GetAnomaly%20Struct%20Array) (Variables|Default|GetAnomaly%20index)))) false))
        (Rendering|SetActorHiddenInGame (.AnomalyObject (Utilities|Struct|BreakAnomaly_Struct (Utilities|Array|Get(acopy) (Variables|Default|GetAnomaly%20Struct%20Array) (Variables|Default|GetAnomaly%20index)))) false)
        (Collision|SetActorEnableCollision (.AnomalyObject (Utilities|Struct|BreakAnomaly_Struct (Utilities|Array|Get(acopy) (Variables|Default|GetAnomaly%20Struct%20Array) (Variables|Default|GetAnomaly%20index)))) true)
        (Math|Integer|IncrementInt (Variables|Default|GetAnomaly%20index)
          (:%20%20
            (CallFunction|Reset)))
        (else
          (Variables|Default|SetCurrent%20floor%20is%20an%20anomaly false)
          (CallFunction|Reset))))))

(event Custom|Turn%20on%20easy%20mode
  (Variables|Default|SetEasy%20mode true))

(event EventBeginPlay
  ;[0 0 0] At begin play, hide the anomalies, then shuffle the array
  (for _array_element (Variables|Default|GetAnomaly%20Struct%20Array)
    (Rendering|SetActorHiddenInGame (.AnomalyObject (Utilities|Struct|BreakAnomaly_Struct _array_element)) true)
    (Collision|SetActorEnableCollision (.AnomalyObject (Utilities|Struct|BreakAnomaly_Struct _array_element)) false))
  (Utilities|Array|Shuffle (Variables|Default|GetAnomaly%20Struct%20Array)))

(fn ConstructionScript)