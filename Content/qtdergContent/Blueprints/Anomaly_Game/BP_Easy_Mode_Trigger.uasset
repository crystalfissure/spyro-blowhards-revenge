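; Trigger volume that switches the anomaly game into easy mode when the player enters its box.
; The overlap only counts for a BP_Base_Playable's capsule while that player's state matches one specific enum value.
; It fires once, calling TurnOnEasyMode on the level's BP_Anomaly_Game and setting the easy mode message on a Gold_Text child actor.
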(event OnComponentBeginOverlap(Box)
  (params (OverlappedComponent :type Primitive%20Component%20Object%20Reference) (OtherActor :type Actor%20Object%20Reference) (OtherComp :type Primitive%20Component%20Object%20Reference) (OtherBodyIndex :type Integer) (bFromSweep :type Boolean) (SweepResult :type Hit%20Result%20Structure%20%28by%20ref%29))
  (bind _asbp_base_playable (Utilities|Casting|CastToBP_Base_Playable OtherActor))
  (if (and (== (Variables|/Script/Engine.Character|GetCapsuleComponent _asbp_base_playable) OtherComp) (Utilities|Enum|Equal(Enum) (Variables|/Game/SpyroContent/Global_Assets/Global_Characters/Playable_Characters/BP_Base_Playable.BP_Base_Playable_C|GetPlayer_State _asbp_base_playable) "NewEnumerator8"))
    (Utilities|FlowControl|DoOnce false
      (:Completed
        (bind _returnvalue (Actor|GetActorOfClass "/Game/qtdergContent/Blueprints/Anomaly_Game/BP_Anomaly_Game.BP_Anomaly_Game_C"))
        (Default|TurnonEasyMode _returnvalue)
        (bind _asgold_text (Utilities|Casting|CastToGold_Text (Variables|/Script/Engine.ChildActorComponent|GetChildActor (Variables|Default|GetEasy%20Mode%20Text%20Actor))))
        (Default|SetText _asgold_text (Variables|Default|GetEasy%20Mode%20Text))))))

(fn ConstructionScript)