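; Customizable fairy Blueprint that applies its color scheme and visible parts to a single mesh on BeginPlay.
; Dynamic material instances tint the skin, dress, lips, eyes, brows, hair and translucent wings from per-part color and brightness variables.
; Unused parts (dragon wings, helmet, shield, infinity symbol, dress overlap) are hidden by swapping in an invisible material, as is the hairstyle not selected by BigPonytail.
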(event EventBeginPlay
  (bind _mesh (Variables|Character|GetMesh))
  (bind _hair_color (Variables|Default|GetHair%20color))
  (bind _mesh_2 (Variables|Character|GetMesh))
  (bind _hair_brightness (Variables|Default|GetHair%20Brightness))
  (|CallParentFunction)
  ;[0 0 0] Dragon wings off
  (Rendering|Material|SetMaterial (Variables|Character|GetMesh) 3 "/Game/SpyroContent/Global_Assets/Global_Materials/Material_Instances/Invisible_Mat.Invisible_Mat")
  ;[0 0 0] Wings color
  (bind _returnvalue (Rendering|Material|CreateDynamicMaterialInstance (Variables|Character|GetMesh) 4 "/Game/SpyroContent/Global_Assets/Global_Materials/Material_Instances/Untex_Vertex_Color_2Sided.Untex_Vertex_Color_2Sided" "None" :!class /Script/Engine.PrimitiveComponent))
  (Rendering|Material|SetVectorParameterValue _returnvalue "ColorChange" (Variables|Default|GetWings%20color) :!class /Script/Engine.MaterialInstanceDynamic)
  (Rendering|Material|SetScalarParameterValue _returnvalue "Opacity" 0.3 :!class /Script/Engine.MaterialInstanceDynamic)
  (Rendering|Material|SetScalarParameterValue _returnvalue "Brightness" (Variables|Default|GetWings%20Brightness) :!class /Script/Engine.MaterialInstanceDynamic)
  ;[0 0 0] Helmet off
  (Rendering|Material|SetMaterial (Variables|Character|GetMesh) 12 "/Game/SpyroContent/Global_Assets/Global_Materials/Material_Instances/Invisible_Mat.Invisible_Mat")
  ;[0 0 0] Shield off
  (Rendering|Material|SetMaterial (Variables|Character|GetMesh) 5 "/Game/SpyroContent/Global_Assets/Global_Materials/Material_Instances/Invisible_Mat.Invisible_Mat")
  ;[0 0 0] Infinite symbol off
  (Rendering|Material|SetMaterial (Variables|Character|GetMesh) 2 "/Game/SpyroContent/Global_Assets/Global_Materials/Material_Instances/Invisible_Mat.Invisible_Mat")
  ;[0 0 0] Skin color
  (bind _returnvalue_2 (Rendering|Material|CreateDynamicMaterialInstance (Variables|Character|GetMesh) 6 "/Game/SpyroContent/Global_Assets/Global_Materials/Material_Instances/Untex_Vertex_Color.Untex_Vertex_Color" "None" :!class /Script/Engine.PrimitiveComponent))
  (Rendering|Material|SetVectorParameterValue _returnvalue_2 "ColorChange" (Variables|Default|GetSkin%20color) :!class /Script/Engine.MaterialInstanceDynamic)
  (Rendering|Material|SetScalarParameterValue _returnvalue_2 "Brightness" (Variables|Default|GetSkin%20Brightness) :!class /Script/Engine.MaterialInstanceDynamic)
  ;[0 0 0] Dress color
  (bind _returnvalue_3 (Rendering|Material|CreateDynamicMaterialInstance (Variables|Character|GetMesh) 10 0 "None" :!class /Script/Engine.PrimitiveComponent))
  (Rendering|Material|SetVectorParameterValue _returnvalue_3 "ColorChange" (Variables|Default|GetDress%20color) :!class /Script/Engine.MaterialInstanceDynamic)
  (Rendering|Material|SetScalarParameterValue _returnvalue_3 "Brightness" (Variables|Default|GetDress%20Brightness) :!class /Script/Engine.MaterialInstanceDynamic)
  ;[0 0 0] Lip color
  (bind _returnvalue_4 (Rendering|Material|CreateDynamicMaterialInstance (Variables|Character|GetMesh) 9 "/Game/SpyroContent/Global_Assets/Global_Materials/Material_Instances/Untex_Vertex_Color.Untex_Vertex_Color" "None" :!class /Script/Engine.PrimitiveComponent))
  (Rendering|Material|SetVectorParameterValue _returnvalue_4 "ColorChange" (Variables|Default|GetLip%20color) :!class /Script/Engine.MaterialInstanceDynamic)
  (Rendering|Material|SetScalarParameterValue _returnvalue_4 "Brightness" (Variables|Default|GetLip%20Brightness) :!class /Script/Engine.MaterialInstanceDynamic)
  ;[0 0 0] Eye color
  (bind _returnvalue_5 (Rendering|Material|CreateDynamicMaterialInstance (Variables|Character|GetMesh) 7 "/Game/SpyroContent/Global_Assets/Global_Characters/NPCs/Fairies/Materials/Fairy_Eyes_Mat.Fairy_Eyes_Mat" "None" :!class /Script/Engine.PrimitiveComponent))
  (Rendering|Material|SetVectorParameterValue _returnvalue_5 "ColorChange" (Variables|Default|GetEye%20color) :!class /Script/Engine.MaterialInstanceDynamic)
  (Rendering|Material|SetScalarParameterValue _returnvalue_5 "Brightness" (Variables|Default|GetEye%20Brightness) :!class /Script/Engine.MaterialInstanceDynamic)
  ;[0 0 0] Brows color
  (bind _returnvalue_6 (Rendering|Material|CreateDynamicMaterialInstance (Variables|Character|GetMesh) 11 "/Game/SpyroContent/Global_Assets/Global_Characters/NPCs/Fairies/Materials/Fairy_Eyes_Mat.Fairy_Eyes_Mat" "None" :!class /Script/Engine.PrimitiveComponent))
  (Rendering|Material|SetVectorParameterValue _returnvalue_6 "ColorChange" (Variables|Default|GetBrows%20color) :!class /Script/Engine.MaterialInstanceDynamic)
  (Rendering|Material|SetScalarParameterValue _returnvalue_6 "Brightness" (Variables|Default|GetBrows%20Brightness) :!class /Script/Engine.MaterialInstanceDynamic)
  ;[0 0 0] Hair color
  (if (Variables|Default|GetBig%20ponytail)
    (Rendering|Material|SetMaterial _mesh 1 "/Game/SpyroContent/Global_Assets/Global_Materials/Material_Instances/Invisible_Mat.Invisible_Mat")
    (bind _returnvalue_7 (Rendering|Material|CreateDynamicMaterialInstance _mesh_2 0 "/Game/SpyroContent/Global_Assets/Global_Materials/Material_Instances/Untex_Vertex_Color.Untex_Vertex_Color" "None" :!class /Script/Engine.PrimitiveComponent))
    (Rendering|Material|SetVectorParameterValue _returnvalue_7 "ColorChange" _hair_color :!class /Script/Engine.MaterialInstanceDynamic)
    (Rendering|Material|SetScalarParameterValue _returnvalue_7 "Brightness" _hair_brightness :!class /Script/Engine.MaterialInstanceDynamic)
    (else
      (Rendering|Material|SetMaterial _mesh 0 "/Game/SpyroContent/Global_Assets/Global_Materials/Material_Instances/Invisible_Mat.Invisible_Mat")
      (bind _returnvalue_8 (Rendering|Material|CreateDynamicMaterialInstance _mesh_2 1 "/Game/SpyroContent/Global_Assets/Global_Materials/Material_Instances/Untex_Vertex_Color.Untex_Vertex_Color" "None" :!class /Script/Engine.PrimitiveComponent))
      (Rendering|Material|SetVectorParameterValue _returnvalue_8 "ColorChange" _hair_color :!class /Script/Engine.MaterialInstanceDynamic)
      (Rendering|Material|SetScalarParameterValue _returnvalue_8 "Brightness" _hair_brightness :!class /Script/Engine.MaterialInstanceDynamic)))
  (bind _returnvalue_9 (Rendering|Material|CreateDynamicMaterialInstance (Variables|Character|GetMesh) 8 "/Game/SpyroContent/Global_Assets/Global_Materials/Material_Instances/Untex_Vertex_Color.Untex_Vertex_Color" "None" :!class /Script/Engine.PrimitiveComponent))
  (Rendering|Material|SetVectorParameterValue _returnvalue_9 "ColorChange" (Variables|Default|GetHair%20color) :!class /Script/Engine.MaterialInstanceDynamic)
  (Rendering|Material|SetScalarParameterValue _returnvalue_9 "Brightness" (Variables|Default|GetHair%20Brightness) :!class /Script/Engine.MaterialInstanceDynamic)
  ;[0 0 0] Dress overlap for super fairies (off)
  (Rendering|Material|SetMaterial (Variables|Character|GetMesh) 13 "/Game/SpyroContent/Global_Assets/Global_Materials/Material_Instances/Invisible_Mat.Invisible_Mat"))

(event Collision|EventActorBeginOverlap
  (params (OtherActor :type Actor%20Object%20Reference)))

(event EventTick
  (params (DeltaSeconds :type Float%20%28single-precision%29))
  (|CallParentFunction DeltaSeconds) ; This node is disabled and will not be called.\nDrag off pins to build functionality.
)

(fn ConstructionScript
  (|CallParentFunction))