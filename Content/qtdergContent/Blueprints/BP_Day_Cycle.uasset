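; BP_Day_Cycle runs an endless day/night cycle by blending a vertex color parameter on its static mesh's material.
; On BeginPlay it creates a dynamic instance of the multi-vertex-color level geometry material and sets the speed of both transition timelines.
; Day and Night events each wait for their configurable length, play a timeline that drives "Vertex Color Lerp", then call each other when it finishes.
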(event Custom|Day
  (Utilities|FlowControl|Delay (Variables|Default|GetDay%20length))
  (bind _newtrack_0 (Timeline|Day%20to%20night%20transition%20timeline PlayFromStart)
    (:Update
      (Rendering|Material|SetScalarParameterValue (Variables|Default|GetMatInstance) "Vertex Color Lerp" _newtrack_0 :!class /Script/Engine.MaterialInstanceDynamic))
    (:Finished
      (CallFunction|Night))))

(event Custom|Night
  (Utilities|FlowControl|Delay (Variables|Default|GetNight%20length))
  (bind _newtrack_0 (Timeline|Night%20to%20day%20transition%20timeline PlayFromStart)
    (:Update
      (Rendering|Material|SetScalarParameterValue (Variables|Default|GetMatInstance) "Vertex Color Lerp" _newtrack_0 :!class /Script/Engine.MaterialInstanceDynamic))
    (:Finished
      (CallFunction|Day))))

(event EventBeginPlay
  (bind _returnvalue (Rendering|Material|CreateDynamicMaterialInstance (Variables|Default|GetStaticMesh) 0 "/Game/qtdergContent/Test/Level_Geometry_MultiVertexColor_Mat_Inst.Level_Geometry_MultiVertexColor_Mat_Inst" "None" :!class /Script/Engine.PrimitiveComponent))
  (Variables|Default|SetMatInstance _returnvalue)
  (Components|Timeline|SetPlayRate (Variables|Default|GetDay%20to%20night%20transition%20timeline) (Variables|Default|GetDay%20to%20night%20transition%20speed))
  (Components|Timeline|SetPlayRate (Variables|Default|GetNight%20to%20day%20transition%20timeline) (Variables|Default|GetNight%20to%20day%20transition%20speed))
  (CallFunction|Day))

(fn ConstructionScript)