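; Trigger volume that teleports the playable character to a spawn point and can pause or unpause the music.
; When the player's capsule overlaps the Box, the actor moves to the SpawnLocation transform with physics teleport.
; It then calls PauseUnpauseMusic using the StopMusic and FastFade settings and resets the player's camera.
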(event OnComponentBeginOverlap(Box)
  (params (OverlappedComponent :type Primitive%20Component%20Object%20Reference) (OtherActor :type Actor%20Object%20Reference) (OtherComp :type Primitive%20Component%20Object%20Reference) (OtherBodyIndex :type Integer) (bFromSweep :type Boolean) (SweepResult :type Hit%20Result%20Structure%20%28by%20ref%29))
  (bind _spawn_location (Variables|Default|GetSpawn%20Location))
  (bind _returnvalue (Transformation|GetWorldTransform _spawn_location))
  (bind _asbp_base_playable (Utilities|Casting|CastToBP_Base_Playable OtherActor))
  (if (== (Variables|/Script/Engine.Character|GetCapsuleComponent _asbp_base_playable) OtherComp)
    (Transformation|SetActorLocationAndRotation _asbp_base_playable (.location _returnvalue) (.rotation _returnvalue) false true)
    (CallFunction|Pause/UnpauseMusic self (Variables|Default|GetStop%20music) (Variables|Default|GetFast%20Fade))
    (Default|InvokedResetCamera _asbp_base_playable)))

(event EventBeginPlay)

(event Collision|EventActorBeginOverlap
  (params (OtherActor :type Actor%20Object%20Reference)))

(event EventTick
  (params (DeltaSeconds :type Float%20%28single-precision%29)))

(fn ConstructionScript)