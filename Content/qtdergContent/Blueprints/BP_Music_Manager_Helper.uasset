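; BP_Music_Manager_Helper is a level helper that decides what the Music_Manager plays when a track finishes.
; On BeginPlay it finds the manager, clears its ManuallyFadedOut flag and binds ManageMusic to the audio-finished event.
; Unless manually faded out, ManageMusic restarts the music, first switching tracks if the level has alternates.
; Alternates either flip-flop between the first two MusicList entries or use a random index, whose upper bound is the list length.
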(event Custom|Manage%20Music
  (bind _self self)
  (bind _self_2 self)
  (if (not (Variables|/Game/SpyroContent/Global_Assets/Global_Level_Items/Music_Manager.Music_Manager_C|GetManually%20faded%20out (Variables|Default|GetMusic%20Manager%20Ref)))
    (if (Variables|Default|GetLevel%20Has%20Alternate%20Music)
      (if (Variables|Default|GetFlip%20Flopping%20Alternates)
        (bind _isa (Utilities|FlowControl|FlipFlop)
          (:A
            _)
          (:B
            _))
        (CallFunction|ChangeMusic _self_2 (select _isa (Utilities|Array|Get(acopy) (Variables|Default|GetMusic%20List) 1) (Utilities|Array|Get(acopy) (Variables|Default|GetMusic%20List))))
        (CallFunction|RestartMusic _self_2)
        (else
          (CallFunction|ChangeMusic _self (Utilities|Array|Get(acopy) (Variables|Default|GetMusic%20List) (Math|Random|RandomIntegerinRange 0 (Utilities|Array|Length (Variables|Default|GetMusic%20List)))))
          (CallFunction|RestartMusic _self)))
      (else
        (CallFunction|RestartMusic self)))))

(event EventBeginPlay
  (bind _returnvalue (Actor|GetActorOfClass "/Game/SpyroContent/Global_Assets/Global_Level_Items/Music_Manager.Music_Manager_C"))
  (Utilities|IsValid _returnvalue
    (:Is%20Valid
      (EventDispatchers|BindEventtoOnAudioFinished (Variables|/Game/SpyroContent/Global_Assets/Global_Level_Items/Music_Manager.Music_Manager_C|GetAudio _returnvalue) (delegate Custom|Manage%20Music))
      (Variables|Default|SetMusic%20Manager%20Ref _returnvalue)
      (Variables|/Game/SpyroContent/Global_Assets/Global_Level_Items/Music_Manager.Music_Manager_C|SetManually%20faded%20out _returnvalue false))))

(fn ConstructionScript)