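; Lava hazard that repeatedly shocks playable characters whose capsule touches its Hitbox.
; Overlap triggers a shock, then delayed self-calling events repeat it while overlap lasts, with a cooldown flag gating new entries.
; Each shock skips invincible or state-exempt players, may reset environmental state and rotation, deals damage, fires DealtDamage and launches the player vertically (noted as unreliable).
; BeginPlay copies the Hitbox mesh onto Collision.
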(event OnComponentBeginOverlap(Hitbox)
  (params (OverlappedComponent :type Primitive%20Component%20Object%20Reference) (OtherActor :type Actor%20Object%20Reference) (OtherComp :type Primitive%20Component%20Object%20Reference) (OtherBodyIndex :type Integer) (bFromSweep :type Boolean) (SweepResult :type Hit%20Result%20Structure%20%28by%20ref%29))
  (Variables|Default|SetOther%20Actor OtherActor)
  (Variables|Default|SetOther%20Comp OtherComp)
  (Variables|Default|SetisOverlapping true)
  (if (Variables|Default|GetCan%20I%20Shock%20The%20Player?)
    (CallFunction|ShockthePlayer OtherActor OtherComp)
    (Variables|Default|SetCan%20I%20Shock%20The%20Player? false)
    (CallFunction|CanShockthePlayerAgain)
    (Utilities|FlowControl|Delay (Variables|Default|GetShock%20Again%20Delay))
    (CallFunction|ShouldIShockPlayerAgain?)))

(event OnComponentEndOverlap(Hitbox)
  (params (OverlappedComponent :type Primitive%20Component%20Object%20Reference) (OtherActor :type Actor%20Object%20Reference) (OtherComp :type Primitive%20Component%20Object%20Reference) (OtherBodyIndex :type Integer))
  (bind _asbp_base_playable (Utilities|Casting|CastToBP_Base_Playable OtherActor))
  (if (== (Variables|/Script/Engine.Character|GetCapsuleComponent _asbp_base_playable) OtherComp)
    (Variables|Default|SetisOverlapping false)))

(event Custom|Should%20I%20Shock%20Player%20Again?
  (if (Variables|Default|GetisOverlapping)
    (CallFunction|ShockthePlayer (Variables|Default|GetOther%20Actor) (Variables|Default|GetOther%20Comp))
    (Variables|Default|SetCan%20I%20Shock%20The%20Player? false)
    (CallFunction|CanShockthePlayerAgain)
    (Utilities|FlowControl|Delay (Variables|Default|GetShock%20Again%20Delay))
    (CallFunction|ShouldIShockPlayerAgain?)))

(event Custom|Can%20Shock%20The%20Player%20Again
  (Utilities|FlowControl|Delay (Variables|Default|GetShock%20Again%20Delay%202))
  (Variables|Default|SetCan%20I%20Shock%20The%20Player? true))

(event EventBeginPlay
  (Components|StaticMesh|SetStaticMesh (Variables|Default|GetCollision) (Variables|/Script/Engine.StaticMeshComponent|GetStaticMesh (Variables|Default|GetHitbox))))

(fn ConstructionScript)

(fn ShockthePlayer
  (params (Player%20Ref :type Object%20Object%20Reference) (Comp%20Ref :type Object%20Object%20Reference))
  (bind _asbp_base_playable (Utilities|Casting|CastToBP_Base_Playable Player%20Ref))
  (if (Math|Boolean|ANDBoolean (== (Variables|/Script/Engine.Character|GetCapsuleComponent _asbp_base_playable) Comp%20Ref) (not (Utilities|Enum|Equal(Enum) (Variables|/Game/SpyroContent/Global_Assets/Global_Characters/Playable_Characters/BP_Base_Playable.BP_Base_Playable_C|GetPlayer_State _asbp_base_playable) "NewEnumerator11")) (not (Variables|/Game/SpyroContent/Global_Assets/Global_Characters/Playable_Characters/BP_Base_Playable.BP_Base_Playable_C|GetCHEAT_Invincibility _asbp_base_playable)) (not (Variables|/Game/SpyroContent/Global_Assets/Global_Characters/Playable_Characters/BP_Base_Playable.BP_Base_Playable_C|GetSuperinvincibility _asbp_base_playable)))
    (if (Utilities|Enum|Equal(Enum) (Variables|/Game/SpyroContent/Global_Assets/Global_Characters/Playable_Characters/BP_Base_Playable.BP_Base_Playable_C|GetEnvironmental_State _asbp_base_playable) "NewEnumerator1")
      (Variables|/Game/SpyroContent/Global_Assets/Global_Characters/Playable_Characters/BP_Base_Playable.BP_Base_Playable_C|SetEnvironmental_State _asbp_base_playable "NewEnumerator0")
      (Transformation|SetActorRotation _asbp_base_playable (Math|Rotator|MakeRotator 0.0 0.0 (.yaw (Transformation|GetActorRotation _asbp_base_playable)))))
    (Default|ResetDamage _asbp_base_playable)
    (Default|DealDamage (Variables|/Game/SpyroContent/Global_Assets/Global_Characters/Playable_Characters/BP_Base_Playable.BP_Base_Playable_C|GetDamageable _asbp_base_playable) "NewEnumerator3" "0, 0, 0" false self false)
    (Default|CallDealtDamage)
    ;[0 0 0] This doesn't always work
    (Character|LaunchCharacter _asbp_base_playable (Math|Vector|MakeVector 0.0 0.0 (Variables|Default|GetLaunch%20Z%20Velocity)) false false)))