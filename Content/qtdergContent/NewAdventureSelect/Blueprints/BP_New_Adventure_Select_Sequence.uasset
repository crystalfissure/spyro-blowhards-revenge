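; Camera actor that plays the looping background showcase and music for the New Adventure Select screen.
; Each cycle applies a shuffled sequence entry to BP_Level_Mesh's four meshes, places the camera and drifts it via timeline between timed fades.
; The saved MusicVibe (random without a save) picks a shuffled track list, advanced through Music_Manager when audio finishes or SkipMusic fires.
; DebugSequence pins the showcase to one entry.
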(event Custom|Skip%20Music
  (bind _self self)
  (if (> (- (Variables|Default|GetMusic%20int) -1) (Utilities|Array|Length (Variables|Default|GetMusic)))
    (Variables|Default|SetMusic%20int 0))
  (CallFunction|ChangeMusic _self (Utilities|Array|Get(acopy) (Variables|Default|GetMusic) (Variables|Default|GetMusic%20int)))
  (CallFunction|RestartMusic _self)
  (Math|Integer|IncrementInt (Variables|Default|GetMusic%20int)))

(event Custom|Cycle
  (bind _level_mesh_actor (Variables|Default|GetLevel%20Mesh%20Actor))
  (if (not (Variables|Default|GetDebug%20sequence))
    (if (> (- (Variables|Default|GetCycle%20Int) -1) (Utilities|Array|Length (Variables|Default|GetSequence%20array)))
      (Variables|Default|SetCycle%20Int 0)
      (Utilities|Array|Shuffle (Variables|Default|GetSequence%20array))))
  (Components|StaticMesh|SetStaticMesh (Variables|/Game/qtdergContent/NewAdventureSelect/Blueprints/BP_Level_Mesh.BP_Level_Mesh_C|GetMesh%201 _level_mesh_actor) (.LevelMesh1 (Utilities|Struct|BreakNew_Adventure_Select_Sequence_Struct (Utilities|Array|Get(acopy) (Variables|Default|GetSequence%20array) (select (Variables|Default|GetDebug%20sequence) (Variables|Default|GetDebug%20sequence%20index) (Variables|Default|GetCycle%20Int))))))
  (Components|StaticMesh|SetStaticMesh (Variables|/Game/qtdergContent/NewAdventureSelect/Blueprints/BP_Level_Mesh.BP_Level_Mesh_C|GetMesh%202 _level_mesh_actor) (.LevelMesh2 (Utilities|Struct|BreakNew_Adventure_Select_Sequence_Struct (Utilities|Array|Get(acopy) (Variables|Default|GetSequence%20array) (select (Variables|Default|GetDebug%20sequence) (Variables|Default|GetDebug%20sequence%20index) (Variables|Default|GetCycle%20Int))))))
  (Components|StaticMesh|SetStaticMesh (Variables|/Game/qtdergContent/NewAdventureSelect/Blueprints/BP_Level_Mesh.BP_Level_Mesh_C|GetMesh%203 _level_mesh_actor) (.LevelMesh3 (Utilities|Struct|BreakNew_Adventure_Select_Sequence_Struct (Utilities|Array|Get(acopy) (Variables|Default|GetSequence%20array) (select (Variables|Default|GetDebug%20sequence) (Variables|Default|GetDebug%20sequence%20index) (Variables|Default|GetCycle%20Int))))))
  (Components|StaticMesh|SetStaticMesh (Variables|/Game/qtdergContent/NewAdventureSelect/Blueprints/BP_Level_Mesh.BP_Level_Mesh_C|GetMesh%204 _level_mesh_actor) (.LevelMesh4 (Utilities|Struct|BreakNew_Adventure_Select_Sequence_Struct (Utilities|Array|Get(acopy) (Variables|Default|GetSequence%20array) (select (Variables|Default|GetDebug%20sequence) (Variables|Default|GetDebug%20sequence%20index) (Variables|Default|GetCycle%20Int))))))
  (Transformation|SetActorTransform (.InitialCameraTransform (Utilities|Struct|BreakNew_Adventure_Select_Sequence_Struct (Utilities|Array|Get(acopy) (Variables|Default|GetSequence%20array) (select (Variables|Default|GetDebug%20sequence) (Variables|Default|GetDebug%20sequence%20index) (Variables|Default|GetCycle%20Int))))))
  (Variables|Default|SetCurrent%20camera%20movement%20direction (.CameraMovementDirection (Utilities|Struct|BreakNew_Adventure_Select_Sequence_Struct (Utilities|Array|Get(acopy) (Variables|Default|GetSequence%20array) (select (Variables|Default|GetDebug%20sequence) (Variables|Default|GetDebug%20sequence%20index) (Variables|Default|GetCycle%20Int))))))
  (Variables|Default|SetCamera%20move%20speed%20multiplier (.CameraMoveSpeed (Utilities|Struct|BreakNew_Adventure_Select_Sequence_Struct (Utilities|Array|Get(acopy) (Variables|Default|GetSequence%20array) (select (Variables|Default|GetDebug%20sequence) (Variables|Default|GetDebug%20sequence%20index) (Variables|Default|GetCycle%20Int))))))
  (CallFunction|CameraMovement)
  (CameraFades|StartCameraFade :self (Game|GetPlayerCameraManager 0) :FromAlpha 1.0 :Duration (Variables|Default|GetCamera%20fade%20time) :bHoldWhenFinished true)
  (Utilities|FlowControl|Delay (Variables|Default|GetCamera%20fade%20time))
  (Utilities|FlowControl|Delay (Variables|Default|GetCycle%20delay))
  (Math|Integer|IncrementInt (Variables|Default|GetCycle%20Int)
    (:%20%20
      (CameraFades|StartCameraFade :self (Game|GetPlayerCameraManager 0) :ToAlpha 1.0 :Duration (Variables|Default|GetCamera%20fade%20time) :bHoldWhenFinished true)
      (Utilities|FlowControl|Delay (Variables|Default|GetCamera%20fade%20time))
      (CallFunction|Cycle))))

(event Custom|Manage%20Music
  (bind _self self)
  (if (> (- (Variables|Default|GetMusic%20int) -1) (Utilities|Array|Length (Variables|Default|GetMusic)))
    (Variables|Default|SetMusic%20int 0))
  (CallFunction|ChangeMusic _self (Utilities|Array|Get(acopy) (Variables|Default|GetMusic) (Variables|Default|GetMusic%20int)))
  (CallFunction|RestartMusic _self)
  (Math|Integer|IncrementInt (Variables|Default|GetMusic%20int)))

(event Custom|Camera%20Movement
  (Transformation|SetRelativeLocation (Variables|Default|GetCamera) "0, 0, 0" false false)
  (bind _newtrack_0 (Timeline|Timeline_0 PlayFromStart)
    (:Update
      (Transformation|AddRelativeLocation (Variables|Default|GetCamera) (Utilities|Select :Index (Variables|Default|GetCurrent%20camera%20movement%20direction) :NewEnumerator0 (Math|Vector|MakeVector 0.0 0.0 (* (* _newtrack_0 (Utilities|Time|GetWorldDeltaSeconds)) (Variables|Default|GetCamera%20move%20speed%20multiplier))) :NewEnumerator1 (Math|Vector|MakeVector 0.0 0.0 (* (* (* _newtrack_0 (Utilities|Time|GetWorldDeltaSeconds)) (Variables|Default|GetCamera%20move%20speed%20multiplier)) -1.0)) :NewEnumerator2 (Math|Vector|MakeVector (* (* _newtrack_0 (Utilities|Time|GetWorldDeltaSeconds)) (Variables|Default|GetCamera%20move%20speed%20multiplier)) 0.0 0.0) :NewEnumerator3 (Math|Vector|MakeVector (* (* (* _newtrack_0 (Utilities|Time|GetWorldDeltaSeconds)) (Variables|Default|GetCamera%20move%20speed%20multiplier)) -1.0) 0.0 0.0) :NewEnumerator4 (Math|Vector|MakeVector 0.0 (* (* (* _newtrack_0 (Utilities|Time|GetWorldDeltaSeconds)) (Variables|Default|GetCamera%20move%20speed%20multiplier)) -1.0) 0.0) :NewEnumerator5 (Math|Vector|MakeVector 0.0 (* (* _newtrack_0 (Utilities|Time|GetWorldDeltaSeconds)) (Variables|Default|GetCamera%20move%20speed%20multiplier)) 0.0)) false false))))

(event EventBeginPlay
  (if (not (Variables|Default|GetDebug%20sequence))
    (Utilities|Array|Shuffle (Variables|Default|GetSequence%20array)))
  (bind _returnvalue (Actor|GetActorOfClass "/Game/qtdergContent/NewAdventureSelect/Blueprints/BP_Level_Mesh.BP_Level_Mesh_C"))
  (Variables|Default|SetLevel%20Mesh%20Actor _returnvalue)
  (CameraFades|StartCameraFade :self (Game|GetPlayerCameraManager 0) :ToAlpha 1.0 :Duration 0.01 :bHoldWhenFinished true)
  (Game|Player|SetViewTargetwithBlend (Game|GetPlayerController 0) self 0.0 "VTBlend_Linear" 0.0 false)
  (bind _returnvalue_2 (SaveGame|LoadGamefromSlot "Adventure_Select_Savedata"))
  (bind _asadventure_select_save_data (Utilities|Casting|CastToAdventure_Select_SaveData _returnvalue_2)
    (:then
      (switch Utilities|FlowControl|Switch|SwitchonMusic_Vibes (Variables|/Game/qtdergContent/NewAdventureSelect/Blueprints/Adventure_Select_SaveData.Adventure_Select_SaveData_C|GetMusic%20Vibe _asadventure_select_save_data)
        (:NewEnumerator0
          (switch int (Math|Random|RandomIntegerinRange 0 2) :!label _label
            (:0
              (Variables|Default|SetMusic (Variables|Default|GetMusic%20Classic) :!label _label_2))
            (:1
              (Variables|Default|SetMusic (Variables|Default|GetMusic%20ETD/Electro) :!label _label_3))
            (:2
              (Variables|Default|SetMusic (Variables|Default|GetMusic%20Relaxing) :!label _label_4))))
        (:NewEnumerator1
          (goto _label_2))
        (:NewEnumerator2
          (goto _label_3))
        (:NewEnumerator3
          (goto _label_4))
        (:NewEnumerator4
          (Utilities|Array|AppendArray (Variables|Default|GetMusic) (Variables|Default|GetMusic%20Classic))
          (Utilities|Array|AppendArray (Variables|Default|GetMusic) (Variables|Default|GetMusic%20ETD/Electro))
          (Utilities|Array|AppendArray (Variables|Default|GetMusic) (Variables|Default|GetMusic%20Relaxing)))))
    (:CastFailed
      (goto _label)))
  (Utilities|Array|Shuffle (Variables|Default|GetMusic))
  (bind _returnvalue_3 (Actor|GetActorOfClass "/Game/SpyroContent/Global_Assets/Global_Level_Items/Music_Manager.Music_Manager_C"))
  (Utilities|IsValid _returnvalue_3
    (:Is%20Valid
      (EventDispatchers|BindEventtoOnAudioFinished (Variables|/Game/SpyroContent/Global_Assets/Global_Level_Items/Music_Manager.Music_Manager_C|GetAudio _returnvalue_3) (delegate Custom|Manage%20Music))
      (CallFunction|ManageMusic))
    (:Is%20Not%20Valid
      _))
  (CallFunction|Cycle))

(fn ConstructionScript)