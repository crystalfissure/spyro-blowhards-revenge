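; Blue star pickup that gives Spyro a Superfly speed boost when touched.
; When a playable character's capsule overlaps its box, it plays a sound and hides, then reappears after a short delay for reuse.
; The boost adds BoostAmount to SuperflySpeedup only if Spyro has Superfly, normal or cheat, and is in one specific player state.
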(event OnComponentBeginOverlap(Box)
  (params (OverlappedComponent :type Primitive%20Component%20Object%20Reference) (OtherActor :type Actor%20Object%20Reference) (OtherComp :type Primitive%20Component%20Object%20Reference) (OtherBodyIndex :type Integer) (bFromSweep :type Boolean) (SweepResult :type Hit%20Result%20Structure%20%28by%20ref%29))
  (bind _asbp_base_playable (Utilities|Casting|CastToBP_Base_Playable OtherActor))
  (if (and (== (Variables|/Script/Engine.Character|GetCapsuleComponent _asbp_base_playable) OtherComp) (not (Variables|Rendering|GetbHidden)))
    (Audio|PlaySoundatLocation "/Game/SpyroContent/Global_Assets/Global_Level_Items/Blue_Star/blue_star_sfx.blue_star_sfx" (Transformation|GetActorLocation) "0, 0, 0" 1.0 1.0 0.0 0 0 0)
    (Rendering|SetActorHiddenInGame true)
    (bind _asbp_spyro (Utilities|Casting|CastToBP_Spyro _asbp_base_playable)
      (:then
        (if (and (or (Variables|/Game/SpyroContent/Global_Assets/Global_Characters/Playable_Characters/Spyro/BP_Spyro.BP_Spyro_C|GetSuperfly _asbp_spyro) (Variables|/Game/SpyroContent/Global_Assets/Global_Characters/Playable_Characters/Spyro/BP_Spyro.BP_Spyro_C|GetCHEAT_Superfly _asbp_spyro)) (Utilities|Enum|Equal(Enum) (Variables|/Game/SpyroContent/Global_Assets/Global_Characters/Playable_Characters/BP_Base_Playable.BP_Base_Playable_C|GetPlayer_State _asbp_spyro) "NewEnumerator1"))
          (Variables|/Game/SpyroContent/Global_Assets/Global_Characters/Playable_Characters/Spyro/BP_Spyro.BP_Spyro_C|SetSuperfly_Speedup _asbp_spyro (+ (Variables|/Game/SpyroContent/Global_Assets/Global_Characters/Playable_Characters/Spyro/BP_Spyro.BP_Spyro_C|GetSuperfly_Speedup _asbp_spyro) (Variables|Default|GetBoost%20Amount)))))
      (:CastFailed
        _))
    (Utilities|FlowControl|Delay 0.75)
    (Rendering|SetActorHiddenInGame false)))

(event EventBeginPlay)

(event Collision|EventActorBeginOverlap
  (params (OtherActor :type Actor%20Object%20Reference)))

(event EventTick
  (params (DeltaSeconds :type Float%20%28single-precision%29)))

(fn ConstructionScript)