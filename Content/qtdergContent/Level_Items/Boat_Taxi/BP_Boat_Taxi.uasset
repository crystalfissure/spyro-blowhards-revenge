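; Boat taxi actor that moves its boat mesh continuously along a spline path in the level.
; Each tick advances a distance by movement speed and sets the mesh's location and rotation from the spline, with a yaw offset.
; The distance resets to zero near the spline's end, restarting the route from the beginning.
; On BeginPlay, a boat flagged as Captain Moby has a 1-in-16 chance of playing a looping animation on its captain.
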(event EventBeginPlay
  (if (Variables|Default|GetIs%20Captain%20Moby)
    (if (== (Math|Random|RandomIntegerinRange 0 15) 7)
      (Components|Animation|PlayAnimation (Variables|Default|GetCaptain) 0 true))))

(event EventTick
  (params (DeltaSeconds :type Float%20%28single-precision%29))
  (Variables|Default|SetCurrentSplineDistance (+ (Variables|Default|GetCurrentSplineDistance) (* (Variables|Default|GetMovementSpeed) DeltaSeconds)))
  (if (>= (+ (Variables|Default|GetCurrentSplineDistance) (* (Variables|Default|GetMovementSpeed) DeltaSeconds)) (Spline|GetSplineLength (Variables|Default|GetSplinePath)))
    (Variables|Default|SetCurrentSplineDistance 0.0)
    (else
      (Transformation|SetWorldLocation (Variables|Default|GetBoat_Mesh) (Spline|GetLocationatDistanceAlongSpline (Variables|Default|GetSplinePath) (Variables|Default|GetCurrentSplineDistance) "World") false false)
      (Transformation|SetRelativeRotation (Variables|Default|GetBoat_Mesh) (Math|Rotator|MakeRotator (.Roll (Math|Rotator|BreakRotator (Spline|GetRotationatDistanceAlongSpline (Variables|Default|GetSplinePath) (Variables|Default|GetCurrentSplineDistance) "World"))) (.Pitch (Math|Rotator|BreakRotator (Spline|GetRotationatDistanceAlongSpline (Variables|Default|GetSplinePath) (Variables|Default|GetCurrentSplineDistance) "World"))) (- (.Yaw (Math|Rotator|BreakRotator (Spline|GetRotationatDistanceAlongSpline (Variables|Default|GetSplinePath) (Variables|Default|GetCurrentSplineDistance) "World"))) (Variables|Default|GetZ%20Rotation%20offset))) false false))))

(fn ConstructionScript)