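; Level item mirror that toggles Spyro's mirror mode when the player walks into its Box trigger.
; Only a playable character's capsule counts; if it is Spyro, he is teleported to the SpawnPoint transform and his camera resets instantly.
; A DoOnce gate blocks re-triggering until a short delay reopens it, though a non-Spyro playable closes it without scheduling that reset.
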(event OnComponentBeginOverlap(Box)
  (params (OverlappedComponent :type Primitive%20Component%20Object%20Reference) (OtherActor :type Actor%20Object%20Reference) (OtherComp :type Primitive%20Component%20Object%20Reference) (OtherBodyIndex :type Integer) (bFromSweep :type Boolean) (SweepResult :type Hit%20Result%20Structure%20%28by%20ref%29))
  (bind _asbp_base_playable (Utilities|Casting|CastToBP_Base_Playable OtherActor))
  (if (== (Variables|/Script/Engine.Character|GetCapsuleComponent _asbp_base_playable) OtherComp)
    (Utilities|FlowControl|DoOnce false
      (:Completed
        (bind _asbp_spyro (Utilities|Casting|CastToBP_Spyro _asbp_base_playable))
        (Default|ToggleMirrorMode _asbp_spyro)
        (Transformation|SetActorTransform _asbp_spyro (Transformation|GetWorldTransform (Variables|Default|GetSpawnPoint)) false true)
        (Default|InstantResetCamera _asbp_spyro)
        (Utilities|FlowControl|Delay 1.0)
        (CallFunction|CanUseMirrorAgain)))))

(event Custom|Can%20Use%20Mirror%20Again
  (Utilities|FlowControl|DoOnce false) ; enters at Reset
)

(fn ConstructionScript)