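; Arachnophobia button that kills every spider, egg sac and nest of the listed classes in the level, enabled once its linked NPC finishes talking.
; A one-time player capsule overlap in a specific player state triggers super damage on each class, credited to the player.
; It binds to the player's about-to-respawn event to repeat the kill.
; SFX volume is temporarily zeroed through the Universal Save during each purge, then restored.
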(event OnComponentBeginOverlap(Box)
  (params (OverlappedComponent :type Primitive%20Component%20Object%20Reference) (OtherActor :type Actor%20Object%20Reference) (OtherComp :type Primitive%20Component%20Object%20Reference) (OtherBodyIndex :type Integer) (bFromSweep :type Boolean) (SweepResult :type Hit%20Result%20Structure%20%28by%20ref%29))
  (bind _asbp_base_playable (Utilities|Casting|CastToBP_Base_Playable OtherActor))
  (if (and (== (Variables|/Script/Engine.Character|GetCapsuleComponent _asbp_base_playable) OtherComp) (Utilities|Enum|Equal(Enum) (Variables|/Game/SpyroContent/Global_Assets/Global_Characters/Playable_Characters/BP_Base_Playable.BP_Base_Playable_C|GetPlayer_State _asbp_base_playable) "NewEnumerator8"))
    (if (Variables|Default|GetButton%20can%20be%20activated)
      (Utilities|FlowControl|DoOnce false
        (:Completed
          (EventDispatchers|BindEventtoAbouttoRespawn _asbp_base_playable (delegate Custom|Kill%20All%20Spiders))
          (bind _asspyro_universal_save_data (CallFunction|LoadUniversalSave))
          (Variables|Default|SetSaved%20Volume%20SFX (Variables|/Game/SpyroContent/Global_Assets/Global_SaveData/Spyro_Universal_Save_Data.Spyro_Universal_Save_Data_C|GetVolume_SFX _asspyro_universal_save_data))
          (Variables|/Game/SpyroContent/Global_Assets/Global_SaveData/Spyro_Universal_Save_Data.Spyro_Universal_Save_Data_C|SetVolume_SFX _asspyro_universal_save_data 0.0)
          (SaveGame|SaveGametoSlot _asspyro_universal_save_data "Universal Save")
          (CallFunction|LoadUniversalSavedOptions self)
          (Utilities|FlowControl|Delay 1.25)
          (Utilities|FlowControl|Sequence
            (:then_0
              (bind _outactors (Actor|GetAllActorsOfClass "/Game/MrTeaSpoonContent/StandaloneLevels/Enemies/Spiders/Patrol_Dervish_Spider_BP.Patrol_Dervish_Spider_BP_C"))
              (for _array_element _outactors
                (bind _returnvalue (Actor|GetActorOfClass "/Game/SpyroContent/Global_Assets/Global_Characters/Playable_Characters/BP_Base_Playable.BP_Base_Playable_C"))
                (Default|DealDamage (Variables|/Game/SpyroContent/Global_Assets/Global_Characters/AI_Characters/Actors/Base_AICharacter_BP.Base_AICharacter_BP_C|GetDamageable _array_element) "NewEnumerator1" "0, 0, 0" true _returnvalue true)))
            (:then_1
              (bind _outactors_2 (Actor|GetAllActorsOfClass "/Game/MrTeaSpoonContent/StandaloneLevels/Enemies/Spiders/Dervish_Spider_BP.Dervish_Spider_BP_C"))
              (for _array_element_2 _outactors_2
                (bind _returnvalue_2 (Actor|GetActorOfClass "/Game/SpyroContent/Global_Assets/Global_Characters/Playable_Characters/BP_Base_Playable.BP_Base_Playable_C"))
                (Default|DealDamage (Variables|/Game/SpyroContent/Global_Assets/Global_Characters/AI_Characters/Actors/Base_AICharacter_BP.Base_AICharacter_BP_C|GetDamageable _array_element_2) "NewEnumerator1" "0, 0, 0" true _returnvalue_2 true)))
            (:then_2
              (bind _outactors_3 (Actor|GetAllActorsOfClass "/Game/MrTeaSpoonContent/StandaloneLevels/Enemies/Spider_Nests/Dervish_Spider_EggSac_BP.Dervish_Spider_EggSac_BP_C"))
              (for _array_element_3 _outactors_3
                (bind _returnvalue_3 (Actor|GetActorOfClass "/Game/SpyroContent/Global_Assets/Global_Characters/Playable_Characters/BP_Base_Playable.BP_Base_Playable_C"))
                (Default|DealDamage (Variables|/Game/SpyroContent/Global_Assets/Global_Level_Items/Treasure_Containers/Treasure_Container_Base_BP.Treasure_Container_Base_BP_C|GetDamageable _array_element_3) "NewEnumerator1" "0, 0, 0" true _returnvalue_3 true)))
            (:then_3
              (bind _outactors_4 (Actor|GetAllActorsOfClass "/Game/MrTeaSpoonContent/StandaloneLevels/Enemies/Spider_Nests/Metal_Metalback_Spider_Nest_BP.Metal_Metalback_Spider_Nest_BP_C"))
              (for _array_element_4 _outactors_4
                (bind _returnvalue_4 (Actor|GetActorOfClass "/Game/SpyroContent/Global_Assets/Global_Characters/Playable_Characters/BP_Base_Playable.BP_Base_Playable_C"))
                (Default|DealDamage (Variables|/Game/SpyroContent/Global_Assets/Global_Level_Items/Treasure_Containers/Treasure_Container_Base_BP.Treasure_Container_Base_BP_C|GetDamageable _array_element_4) "NewEnumerator1" "0, 0, 0" true _returnvalue_4 true)))
            (:then_4
              (bind _outactors_5 (Actor|GetAllActorsOfClass "/Game/MrTeaSpoonContent/StandaloneLevels/Enemies/Spiders/Metal_Spider_BP.Metal_Spider_BP_C"))
              (for _array_element_5 _outactors_5
                (bind _returnvalue_5 (Actor|GetActorOfClass "/Game/SpyroContent/Global_Assets/Global_Characters/Playable_Characters/BP_Base_Playable.BP_Base_Playable_C"))
                (Default|DealDamage (Variables|/Game/SpyroContent/Global_Assets/Global_Characters/AI_Characters/Actors/Base_AICharacter_BP.Base_AICharacter_BP_C|GetDamageable _array_element_5) "NewEnumerator1" "0, 0, 0" true _returnvalue_5 true)))
            (:then_5
              (bind _outactors_6 (Actor|GetAllActorsOfClass "/Game/MrTeaSpoonContent/StandaloneLevels/Enemies/Spider_Nests/Spider_EggSac_BP.Spider_EggSac_BP_C"))
              (for _array_element_6 _outactors_6
                (bind _returnvalue_6 (Actor|GetActorOfClass "/Game/SpyroContent/Global_Assets/Global_Characters/Playable_Characters/BP_Base_Playable.BP_Base_Playable_C"))
                (Default|DealDamage (Variables|/Game/SpyroContent/Global_Assets/Global_Level_Items/Treasure_Containers/Treasure_Container_Base_BP.Treasure_Container_Base_BP_C|GetDamageable _array_element_6) "NewEnumerator1" "0, 0, 0" true _returnvalue_6 true)))
            (:then_6
              (bind _outactors_7 (Actor|GetAllActorsOfClass "/Game/MrTeaSpoonContent/StandaloneLevels/Enemies/Spiders/Spider_ChargeAndAttack_BP.Spider_ChargeAndAttack_BP_C"))
              (for _array_element_7 _outactors_7
                (bind _returnvalue_7 (Actor|GetActorOfClass "/Game/SpyroContent/Global_Assets/Global_Characters/Playable_Characters/BP_Base_Playable.BP_Base_Playable_C"))
                (Default|DealDamage (Variables|/Game/SpyroContent/Global_Assets/Global_Characters/AI_Characters/Actors/Base_AICharacter_BP.Base_AICharacter_BP_C|GetDamageable _array_element_7) "NewEnumerator1" "0, 0, 0" true _returnvalue_7 true)))
            (:then_7
              (bind _outactors_8 (Actor|GetAllActorsOfClass "/Game/MrTeaSpoonContent/StandaloneLevels/Enemies/Spiders/Patrol_Spider_BP.Patrol_Spider_BP_C"))
              (for _array_element_8 _outactors_8
                (bind _returnvalue_8 (Actor|GetActorOfClass "/Game/SpyroContent/Global_Assets/Global_Characters/Playable_Characters/BP_Base_Playable.BP_Base_Playable_C"))
                (Default|DealDamage (Variables|/Game/SpyroContent/Global_Assets/Global_Characters/AI_Characters/Actors/Base_AICharacter_BP.Base_AICharacter_BP_C|GetDamageable _array_element_8) "NewEnumerator1" "0, 0, 0" true _returnvalue_8 true)))
            (:then_8
              (bind _outactors_9 (Actor|GetAllActorsOfClass "/Game/MrTeaSpoonContent/StandaloneLevels/Enemies/Spiders/Spider_StandAndAttackV2_BP.Spider_StandAndAttackV2_BP_C"))
              (for _array_element_9 _outactors_9
                (bind _returnvalue_9 (Actor|GetActorOfClass "/Game/SpyroContent/Global_Assets/Global_Characters/Playable_Characters/BP_Base_Playable.BP_Base_Playable_C"))
                (Default|DealDamage (Variables|/Game/SpyroContent/Global_Assets/Global_Characters/AI_Characters/Actors/Base_AICharacter_BP.Base_AICharacter_BP_C|GetDamageable _array_element_9) "NewEnumerator1" "0, 0, 0" true _returnvalue_9 true)))
            (:then_9
              (bind _outactors_10 (Actor|GetAllActorsOfClass "/Game/MrTeaSpoonContent/StandaloneLevels/Enemies/Spiders/Drop_Spider2_BP.Drop_Spider2_BP_C"))
              (for _array_element_10 _outactors_10
                (bind _returnvalue_10 (Actor|GetActorOfClass "/Game/SpyroContent/Global_Assets/Global_Characters/Playable_Characters/BP_Base_Playable.BP_Base_Playable_C"))
                (Default|DealDamage (Variables|/Game/SpyroContent/Global_Assets/Global_Characters/AI_Characters/Actors/Base_AICharacter_BP.Base_AICharacter_BP_C|GetDamageable _array_element_10) "NewEnumerator1" "0, 0, 0" true _returnvalue_10 true)))
            (:then_10
              (CallFunction|RestoreSFXVolume))))))))

(event Custom|Kill%20All%20Spiders
  (Utilities|FlowControl|Delay 1.0)
  (bind _asspyro_universal_save_data (CallFunction|LoadUniversalSave))
  (Variables|Default|SetSaved%20Volume%20SFX (Variables|/Game/SpyroContent/Global_Assets/Global_SaveData/Spyro_Universal_Save_Data.Spyro_Universal_Save_Data_C|GetVolume_SFX _asspyro_universal_save_data))
  (Variables|/Game/SpyroContent/Global_Assets/Global_SaveData/Spyro_Universal_Save_Data.Spyro_Universal_Save_Data_C|SetVolume_SFX _asspyro_universal_save_data 0.0)
  (SaveGame|SaveGametoSlot _asspyro_universal_save_data "Universal Save")
  (CallFunction|LoadUniversalSavedOptions self)
  (Utilities|FlowControl|Delay 1.25)
  (Utilities|FlowControl|Sequence
    (:then_0
      (bind _outactors (Actor|GetAllActorsOfClass "/Game/MrTeaSpoonContent/StandaloneLevels/Enemies/Spiders/Patrol_Dervish_Spider_BP.Patrol_Dervish_Spider_BP_C"))
      (for _array_element _outactors
        (bind _returnvalue (Actor|GetActorOfClass "/Game/SpyroContent/Global_Assets/Global_Characters/Playable_Characters/BP_Base_Playable.BP_Base_Playable_C"))
        (Default|DealDamage (Variables|/Game/SpyroContent/Global_Assets/Global_Characters/AI_Characters/Actors/Base_AICharacter_BP.Base_AICharacter_BP_C|GetDamageable _array_element) "NewEnumerator1" "0, 0, 0" true _returnvalue true)))
    (:then_1
      (bind _outactors_2 (Actor|GetAllActorsOfClass "/Game/MrTeaSpoonContent/StandaloneLevels/Enemies/Spiders/Dervish_Spider_BP.Dervish_Spider_BP_C"))
      (for _array_element_2 _outactors_2
        (bind _returnvalue_2 (Actor|GetActorOfClass "/Game/SpyroContent/Global_Assets/Global_Characters/Playable_Characters/BP_Base_Playable.BP_Base_Playable_C"))
        (Default|DealDamage (Variables|/Game/SpyroContent/Global_Assets/Global_Characters/AI_Characters/Actors/Base_AICharacter_BP.Base_AICharacter_BP_C|GetDamageable _array_element_2) "NewEnumerator1" "0, 0, 0" true _returnvalue_2 true)))
    (:then_2
      (bind _outactors_3 (Actor|GetAllActorsOfClass "/Game/MrTeaSpoonContent/StandaloneLevels/Enemies/Spider_Nests/Dervish_Spider_EggSac_BP.Dervish_Spider_EggSac_BP_C"))
      (for _array_element_3 _outactors_3
        (bind _returnvalue_3 (Actor|GetActorOfClass "/Game/SpyroContent/Global_Assets/Global_Characters/Playable_Characters/BP_Base_Playable.BP_Base_Playable_C"))
        (Default|DealDamage (Variables|/Game/SpyroContent/Global_Assets/Global_Level_Items/Treasure_Containers/Treasure_Container_Base_BP.Treasure_Container_Base_BP_C|GetDamageable _array_element_3) "NewEnumerator1" "0, 0, 0" true _returnvalue_3 true)))
    (:then_3
      (bind _outactors_4 (Actor|GetAllActorsOfClass "/Game/MrTeaSpoonContent/StandaloneLevels/Enemies/Spider_Nests/Metal_Metalback_Spider_Nest_BP.Metal_Metalback_Spider_Nest_BP_C"))
      (for _array_element_4 _outactors_4
        (bind _returnvalue_4 (Actor|GetActorOfClass "/Game/SpyroContent/Global_Assets/Global_Characters/Playable_Characters/BP_Base_Playable.BP_Base_Playable_C"))
        (Default|DealDamage (Variables|/Game/SpyroContent/Global_Assets/Global_Level_Items/Treasure_Containers/Treasure_Container_Base_BP.Treasure_Container_Base_BP_C|GetDamageable _array_element_4) "NewEnumerator1" "0, 0, 0" true _returnvalue_4 true)))
    (:then_4
      (bind _outactors_5 (Actor|GetAllActorsOfClass "/Game/MrTeaSpoonContent/StandaloneLevels/Enemies/Spiders/Metal_Spider_BP.Metal_Spider_BP_C"))
      (for _array_element_5 _outactors_5
        (bind _returnvalue_5 (Actor|GetActorOfClass "/Game/SpyroContent/Global_Assets/Global_Characters/Playable_Characters/BP_Base_Playable.BP_Base_Playable_C"))
        (Default|DealDamage (Variables|/Game/SpyroContent/Global_Assets/Global_Characters/AI_Characters/Actors/Base_AICharacter_BP.Base_AICharacter_BP_C|GetDamageable _array_element_5) "NewEnumerator1" "0, 0, 0" true _returnvalue_5 true)))
    (:then_5
      (bind _outactors_6 (Actor|GetAllActorsOfClass "/Game/MrTeaSpoonContent/StandaloneLevels/Enemies/Spider_Nests/Spider_EggSac_BP.Spider_EggSac_BP_C"))
      (for _array_element_6 _outactors_6
        (bind _returnvalue_6 (Actor|GetActorOfClass "/Game/SpyroContent/Global_Assets/Global_Characters/Playable_Characters/BP_Base_Playable.BP_Base_Playable_C"))
        (Default|DealDamage (Variables|/Game/SpyroContent/Global_Assets/Global_Level_Items/Treasure_Containers/Treasure_Container_Base_BP.Treasure_Container_Base_BP_C|GetDamageable _array_element_6) "NewEnumerator1" "0, 0, 0" true _returnvalue_6 true)))
    (:then_6
      (bind _outactors_7 (Actor|GetAllActorsOfClass "/Game/MrTeaSpoonContent/StandaloneLevels/Enemies/Spiders/Spider_ChargeAndAttack_BP.Spider_ChargeAndAttack_BP_C"))
      (for _array_element_7 _outactors_7
        (bind _returnvalue_7 (Actor|GetActorOfClass "/Game/SpyroContent/Global_Assets/Global_Characters/Playable_Characters/BP_Base_Playable.BP_Base_Playable_C"))
        (Default|DealDamage (Variables|/Game/SpyroContent/Global_Assets/Global_Characters/AI_Characters/Actors/Base_AICharacter_BP.Base_AICharacter_BP_C|GetDamageable _array_element_7) "NewEnumerator1" "0, 0, 0" true _returnvalue_7 true)))
    (:then_7
      (bind _outactors_8 (Actor|GetAllActorsOfClass "/Game/MrTeaSpoonContent/StandaloneLevels/Enemies/Spiders/Patrol_Spider_BP.Patrol_Spider_BP_C"))
      (for _array_element_8 _outactors_8
        (bind _returnvalue_8 (Actor|GetActorOfClass "/Game/SpyroContent/Global_Assets/Global_Characters/Playable_Characters/BP_Base_Playable.BP_Base_Playable_C"))
        (Default|DealDamage (Variables|/Game/SpyroContent/Global_Assets/Global_Characters/AI_Characters/Actors/Base_AICharacter_BP.Base_AICharacter_BP_C|GetDamageable _array_element_8) "NewEnumerator1" "0, 0, 0" true _returnvalue_8 true)))
    (:then_8
      (bind _outactors_9 (Actor|GetAllActorsOfClass "/Game/MrTeaSpoonContent/StandaloneLevels/Enemies/Spiders/Spider_StandAndAttackV2_BP.Spider_StandAndAttackV2_BP_C"))
      (for _array_element_9 _outactors_9
        (bind _returnvalue_9 (Actor|GetActorOfClass "/Game/SpyroContent/Global_Assets/Global_Characters/Playable_Characters/BP_Base_Playable.BP_Base_Playable_C"))
        (Default|DealDamage (Variables|/Game/SpyroContent/Global_Assets/Global_Characters/AI_Characters/Actors/Base_AICharacter_BP.Base_AICharacter_BP_C|GetDamageable _array_element_9) "NewEnumerator1" "0, 0, 0" true _returnvalue_9 true)))
    (:then_9
      (bind _outactors_10 (Actor|GetAllActorsOfClass "/Game/MrTeaSpoonContent/StandaloneLevels/Enemies/Spiders/Drop_Spider2_BP.Drop_Spider2_BP_C"))
      (for _array_element_10 _outactors_10
        (bind _returnvalue_10 (Actor|GetActorOfClass "/Game/SpyroContent/Global_Assets/Global_Characters/Playable_Characters/BP_Base_Playable.BP_Base_Playable_C"))
        (Default|DealDamage (Variables|/Game/SpyroContent/Global_Assets/Global_Characters/AI_Characters/Actors/Base_AICharacter_BP.Base_AICharacter_BP_C|GetDamageable _array_element_10) "NewEnumerator1" "0, 0, 0" true _returnvalue_10 true)))
    (:then_10
      (CallFunction|RestoreSFXVolume))))

(event Custom|Restore%20SFX%20Volume
  (Utilities|FlowControl|Delay 1.0)
  (bind _asspyro_universal_save_data (CallFunction|LoadUniversalSave))
  (Variables|/Game/SpyroContent/Global_Assets/Global_SaveData/Spyro_Universal_Save_Data.Spyro_Universal_Save_Data_C|SetVolume_SFX _asspyro_universal_save_data (Variables|Default|GetSaved%20Volume%20SFX))
  (SaveGame|SaveGametoSlot _asspyro_universal_save_data "Universal Save")
  (CallFunction|LoadUniversalSavedOptions self))

(event Custom|Activate%20button
  (Variables|Default|SetButton%20can%20be%20activated true))

(event EventBeginPlay
  (EventDispatchers|BindEventtoDoneTalking (Variables|Default|GetNPC%20Ref) (delegate Custom|Activate%20button)))

(fn ConstructionScript)