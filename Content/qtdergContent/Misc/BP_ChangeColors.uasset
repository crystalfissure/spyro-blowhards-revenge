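; BP_ChangeColors continuously animates a material blend on a static mesh, by its name to cycle colors.
; BeginPlay creates five dynamic instances of Level_Geometry_Mat_ForCookies_Inst on the mesh's material slots and starts a timeline.
; The timeline drives each instance's BlendFactor parameter and restarts through StartNextCycle when finished, forming an endless loop.
; CustomEvent_0 stops the timeline.
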(event Custom|StartNextCycle
  (bind _newtrack_0 (Timeline|Timeline_0 PlayFromStart)
    (:Update
      (Rendering|Material|SetScalarParameterValue (stale EventBeginPlay _returnvalue_5) "BlendFactor" _newtrack_0 :!class /Script/Engine.MaterialInstanceDynamic)
      (Rendering|Material|SetScalarParameterValue (stale EventBeginPlay _returnvalue_4) "BlendFactor" _newtrack_0 :!class /Script/Engine.MaterialInstanceDynamic)
      (Rendering|Material|SetScalarParameterValue (stale EventBeginPlay _returnvalue_3) "BlendFactor" _newtrack_0 :!class /Script/Engine.MaterialInstanceDynamic)
      (Rendering|Material|SetScalarParameterValue (stale EventBeginPlay _returnvalue_2) "BlendFactor" _newtrack_0 :!class /Script/Engine.MaterialInstanceDynamic)
      (Rendering|Material|SetScalarParameterValue (stale EventBeginPlay _returnvalue) "BlendFactor" _newtrack_0 :!class /Script/Engine.MaterialInstanceDynamic))
    (:Finished
      (CallFunction|StartNextCycle))))

(event Custom|CustomEvent_0
  (bind _newtrack_0 (Timeline|Timeline_0 Stop)
    (:Update
      (Rendering|Material|SetScalarParameterValue (stale EventBeginPlay _returnvalue_5) "BlendFactor" _newtrack_0 :!class /Script/Engine.MaterialInstanceDynamic)
      (Rendering|Material|SetScalarParameterValue (stale EventBeginPlay _returnvalue_4) "BlendFactor" _newtrack_0 :!class /Script/Engine.MaterialInstanceDynamic)
      (Rendering|Material|SetScalarParameterValue (stale EventBeginPlay _returnvalue_3) "BlendFactor" _newtrack_0 :!class /Script/Engine.MaterialInstanceDynamic)
      (Rendering|Material|SetScalarParameterValue (stale EventBeginPlay _returnvalue_2) "BlendFactor" _newtrack_0 :!class /Script/Engine.MaterialInstanceDynamic)
      (Rendering|Material|SetScalarParameterValue (stale EventBeginPlay _returnvalue) "BlendFactor" _newtrack_0 :!class /Script/Engine.MaterialInstanceDynamic))
    (:Finished
      (CallFunction|StartNextCycle))))

(event EventBeginPlay
  (bind _returnvalue (Rendering|Material|CreateDynamicMaterialInstance (Variables|Default|GetStaticMesh) 0 "/Game/qtdergContent/Misc/Level_Geometry_Mat_ForCookies_Inst.Level_Geometry_Mat_ForCookies_Inst" "None" :!class /Script/Engine.PrimitiveComponent))
  (bind _returnvalue_2 (Rendering|Material|CreateDynamicMaterialInstance (Variables|Default|GetStaticMesh) 1 "/Game/qtdergContent/Misc/Level_Geometry_Mat_ForCookies_Inst.Level_Geometry_Mat_ForCookies_Inst" "None" :!class /Script/Engine.PrimitiveComponent))
  (bind _returnvalue_3 (Rendering|Material|CreateDynamicMaterialInstance (Variables|Default|GetStaticMesh) 2 "/Game/qtdergContent/Misc/Level_Geometry_Mat_ForCookies_Inst.Level_Geometry_Mat_ForCookies_Inst" "None" :!class /Script/Engine.PrimitiveComponent))
  (bind _returnvalue_4 (Rendering|Material|CreateDynamicMaterialInstance (Variables|Default|GetStaticMesh) 3 "/Game/qtdergContent/Misc/Level_Geometry_Mat_ForCookies_Inst.Level_Geometry_Mat_ForCookies_Inst" "None" :!class /Script/Engine.PrimitiveComponent))
  (bind _returnvalue_5 (Rendering|Material|CreateDynamicMaterialInstance (Variables|Default|GetStaticMesh) 4 "/Game/qtdergContent/Misc/Level_Geometry_Mat_ForCookies_Inst.Level_Geometry_Mat_ForCookies_Inst" "None" :!class /Script/Engine.PrimitiveComponent))
  (bind _newtrack_0 (Timeline|Timeline_0 PlayFromStart)
    (:Update
      (Rendering|Material|SetScalarParameterValue _returnvalue_5 "BlendFactor" _newtrack_0 :!class /Script/Engine.MaterialInstanceDynamic)
      (Rendering|Material|SetScalarParameterValue _returnvalue_4 "BlendFactor" _newtrack_0 :!class /Script/Engine.MaterialInstanceDynamic)
      (Rendering|Material|SetScalarParameterValue _returnvalue_3 "BlendFactor" _newtrack_0 :!class /Script/Engine.MaterialInstanceDynamic)
      (Rendering|Material|SetScalarParameterValue _returnvalue_2 "BlendFactor" _newtrack_0 :!class /Script/Engine.MaterialInstanceDynamic)
      (Rendering|Material|SetScalarParameterValue _returnvalue "BlendFactor" _newtrack_0 :!class /Script/Engine.MaterialInstanceDynamic))
    (:Finished
      (CallFunction|StartNextCycle))))

(fn ConstructionScript)