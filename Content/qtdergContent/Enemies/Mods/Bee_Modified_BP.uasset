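; Modified bee enemy that flies forward continuously while bobbing around its spawn height.
; Two timelines alternate up and down with randomized offsets, lerp strength and pauses, sweeping the actor's Z toward each target.
; Tick moves it along its forward vector using FlyingAICharacter's speed, spins it rapidly in yaw while that reports it stuck, and otherwise optionally turns it in clockwise or counterclockwise circles.
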(event Custom|Fly%20Down
  (bind _returnvalue (Transformation|GetActorLocation))
  (Variables|Default|SetTarget%20Height%20Offset (Math|Random|RandomFloatinRange 5.0 1e+01))
  (Variables|Default|SetHeight%20Lerp%20Alpha%20Multiplier (Math|Random|RandomFloatinRange 0.2 1.0))
  (bind _newtrack_0 (Timeline|Timeline_1 PlayFromStart)
    (:Update
      (Transformation|SetActorLocation (Math|Vector|MakeVector (.x _returnvalue) (.y _returnvalue) (Math|Float|Lerp (.z _returnvalue) (- (Variables|Default|GetTarget_Height) (Variables|Default|GetTarget%20Height%20Offset)) (* _newtrack_0 (Variables|Default|GetHeight%20Lerp%20Alpha%20Multiplier)))) true false))
    (:Finished
      (Utilities|FlowControl|Delay (Math|Random|RandomFloatinRange 0.2 1.5))
      (CallFunction|FlyUp))))

(event Custom|Fly%20Up
  (bind _returnvalue (Transformation|GetActorLocation))
  (Variables|Default|SetTarget%20Height%20Offset (Math|Random|RandomFloatinRange 5.0 1e+01))
  (Variables|Default|SetHeight%20Lerp%20Alpha%20Multiplier (Math|Random|RandomFloatinRange 0.2 1.0))
  (bind _newtrack_0 (Timeline|Timeline_0 PlayFromStart)
    (:Update
      (Transformation|SetActorLocation (Math|Vector|MakeVector (.x _returnvalue) (.y _returnvalue) (Math|Float|Lerp (.z _returnvalue) (+ (Variables|Default|GetTarget_Height) (Variables|Default|GetTarget%20Height%20Offset)) (* _newtrack_0 (Variables|Default|GetHeight%20Lerp%20Alpha%20Multiplier)))) true false))
    (:Finished
      (Utilities|FlowControl|Delay (Math|Random|RandomFloatinRange 0.2 1.5))
      (CallFunction|FlyDown))))

(event EventBeginPlay
  (Variables|Default|SetTarget_Height (.z (Transformation|GetActorLocation)))
  (CallFunction|FlyUp))

(event EventTick
  (params (DeltaSeconds :type Float%20%28single-precision%29))
  (Transformation|AddActorWorldOffset (* (Transformation|GetActorForwardVector) (* (Utilities|Time|GetWorldDeltaSeconds) (* (Variables|/Game/SpyroContent/Global_Assets/Global_Components/Child_Components/Flying_AI_Character.Flying_AI_Character_C|GetFlyingSpeed (Variables|Default|GetFlying_AI_Character)) 4.0))) true)
  (bind _returnvalue (Default|IsThisActorStuck? (Variables|Default|GetFlying_AI_Character)))
  (if _returnvalue
    (Transformation|AddActorLocalRotation (Math|Rotator|MakeRotator 0.0 0.0 (* (Utilities|Time|GetWorldDeltaSeconds) 3e+03)) false false)
    (elif (Variables|Default|GetFlying%20in%20Circles)
      (Transformation|AddActorLocalRotation (Math|Rotator|MakeRotator 0.0 0.0 (* (Utilities|Time|GetWorldDeltaSeconds) 2e+02 (select (Variables|Default|GetCounterclockwise) -1.0 1.0))) false false))))

(fn ConstructionScript)