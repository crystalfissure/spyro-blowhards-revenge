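; Base patrol enemy that moves back and forth between its spawn point and MoveTo, optionally flipping its mesh at each end.
; Hurtbox damages players, with optional charge-state exception and self-destruct if they retain hit points; falling players can stomp JumpOn to damage it and bounce, higher while holding jump.
; Successful damage through Damageable stops the patrol and optionally shrinks the mesh; an item-dropper reset clears death and restores scale and rotation.
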(event OnComponentBeginOverlap(JumpOn)
  (params (OverlappedComponent :type Primitive%20Component%20Object%20Reference) (OtherActor :type Actor%20Object%20Reference) (OtherComp :type Primitive%20Component%20Object%20Reference) (OtherBodyIndex :type Integer) (bFromSweep :type Boolean) (SweepResult :type Hit%20Result%20Structure%20%28by%20ref%29))
  (if (Variables|Default|GetCan%20Be%20Jumped%20On)
    (if (not (Variables|Default|GetisDying))
      (bind _asbp_base_playable (Utilities|Casting|CastToBP_Base_Playable OtherActor))
      (if (Math|Boolean|ANDBoolean (Utilities|Enum|Equal(Enum) (Variables|/Game/SpyroContent/Global_Assets/Global_Characters/Playable_Characters/BP_Base_Playable.BP_Base_Playable_C|GetEnvironmental_State _asbp_base_playable) "NewEnumerator2") (< (.Z (Math|Vector|BreakVector (Pawn|Components|CharacterMovement|GetLastUpdateVelocity (Variables|/Script/Engine.Character|GetCharacterMovement _asbp_base_playable)))) 0.0) (not (Utilities|Enum|Equal(Enum) (Variables|/Game/SpyroContent/Global_Assets/Global_Characters/Playable_Characters/BP_Base_Playable.BP_Base_Playable_C|GetPlayer_State _asbp_base_playable) "NewEnumerator8")) (== (Variables|/Script/Engine.Character|GetCapsuleComponent _asbp_base_playable) OtherComp))
        (bind _returnvalue (Default|IsJumpButtonHeldFunction _asbp_base_playable))
        (if _returnvalue
          (Variables|/Script/Engine.MovementComponent|SetVelocity (Variables|/Script/Engine.Character|GetCharacterMovement _asbp_base_playable) (Math|Vector|MakeVector (.X (Math|Vector|BreakVector (Pawn|Components|CharacterMovement|GetLastUpdateVelocity (Variables|/Script/Engine.Character|GetCharacterMovement _asbp_base_playable)))) (.Y (Math|Vector|BreakVector (Pawn|Components|CharacterMovement|GetLastUpdateVelocity (Variables|/Script/Engine.Character|GetCharacterMovement _asbp_base_playable)))) 1.05e+03))
          (else
            (Variables|/Script/Engine.MovementComponent|SetVelocity (Variables|/Script/Engine.Character|GetCharacterMovement _asbp_base_playable) (Math|Vector|MakeVector (.X (Math|Vector|BreakVector (Pawn|Components|CharacterMovement|GetLastUpdateVelocity (Variables|/Script/Engine.Character|GetCharacterMovement _asbp_base_playable)))) (.Y (Math|Vector|BreakVector (Pawn|Components|CharacterMovement|GetLastUpdateVelocity (Variables|/Script/Engine.Character|GetCharacterMovement _asbp_base_playable)))) 7.5e+02))))
        (Default|DealDamage (Variables|Default|GetDamageable) "NewEnumerator0" "0, 0, 0" false _asbp_base_playable true)))))

(event DamageWasSuccessfullyDealt(Damageable)
  (Variables|Default|SetisDying true)
  (CallFunction|DeathSequence))

(event ItemDropperSuccessfullyReset(Drops_Items)
  (bind _initial_rotation (Variables|Default|GetInitial%20Rotation))
  (bind (_roll _pitch _yaw) (Math|Rotator|BreakRotator _initial_rotation))
  (if (Variables|Default|GetisDying)
    (Collision|SetCollisionEnabled (Variables|Default|GetCapsuleComponent) "NoCollision")
    (Variables|Default|SetisDying false)
    (Transformation|SetRelativeScale3D (Variables|Character|GetMesh) (Variables|Default|GetInital%20Scale))
    (Transformation|SetRelativeRotation (Variables|Default|GetCapsuleComponent) (Variables|Default|GetInitial%20Capsule%20Rotation) false false)
    (if (Variables|Default|GetRotateMeshAfterReachingEndPoint)
      (if (Variables|Default|GetMovingToEnd)
        (Transformation|SetRelativeRotation (Variables|Character|GetMesh) _initial_rotation false false)
        (else
          (Transformation|SetRelativeRotation (Variables|Character|GetMesh) (Math|Rotator|MakeRotator _roll _pitch (+ _yaw 1.8e+02)) false false))))))

(event OnComponentBeginOverlap(Hurtbox)
  (params (OverlappedComponent :type Primitive%20Component%20Object%20Reference) (OtherActor :type Actor%20Object%20Reference) (OtherComp :type Primitive%20Component%20Object%20Reference) (OtherBodyIndex :type Integer) (bFromSweep :type Boolean) (SweepResult :type Hit%20Result%20Structure%20%28by%20ref%29))
  (if (not (Variables|Default|GetisDying))
    (bind _asbp_base_playable (Utilities|Casting|CastToBP_Base_Playable OtherActor))
    (if (== (Variables|/Script/Engine.Character|GetCapsuleComponent _asbp_base_playable) OtherComp)
      (if (Variables|Default|GetisChargeable)
        (if (not (Utilities|Enum|Equal(Enum) (Variables|/Game/SpyroContent/Global_Assets/Global_Characters/Playable_Characters/BP_Base_Playable.BP_Base_Playable_C|GetPlayer_State _asbp_base_playable) "NewEnumerator4"))
          (Default|DealDamage (Variables|/Game/SpyroContent/Global_Assets/Global_Characters/Playable_Characters/BP_Base_Playable.BP_Base_Playable_C|GetDamageable _asbp_base_playable) (Variables|Default|GetDamage%20Type) (Transformation|GetActorForwardVector) false self false :!label _label)
          (if (not (== (Variables|/Game/SpyroContent/Global_Assets/Global_Components/Damageable_Com.Damageable_Com_C|GetHit%20Points (Variables|/Game/SpyroContent/Global_Assets/Global_Characters/Playable_Characters/BP_Base_Playable.BP_Base_Playable_C|GetDamageable _asbp_base_playable)) 0))
            (if (Variables|Default|GetSelf%20Destructs%20if%20Player%20Has%20Sparx)
              (Default|DealDamage (Variables|Default|GetDamageable) "NewEnumerator0" "0, 0, 0" false _asbp_base_playable true))))
        (else
          (goto _label))))))

(event Custom|Death%20Sequence
  (Collision|SetCollisionResponsetoChannel (Variables|Default|GetCapsuleComponent) "ECC_Pawn" "ECR_Ignore")
  (if (Variables|Default|GetShrinks%20After%20Dying)
    (bind _newtrack_0 (Timeline|Timeline PlayFromStart)
      (:Update
        (Transformation|SetRelativeScale3D (Variables|Character|GetMesh) (Math|Conversions|ToVector(Float) _newtrack_0))))))

(event EventBeginPlay
  (bind _mesh (Variables|Character|GetMesh))
  (bind _returnvalue (Transformation|GetRelativeTransform _mesh))
  (bind (_location _rotation _scale) (Math|Transform|BreakTransform _returnvalue))
  (|CallParentFunction)
  (Variables|/Game/SpyroContent/Global_Assets/Global_Components/Damageable_Com.Damageable_Com_C|SetObject's%20Hitbox%20Component (Variables|Default|GetDamageable) (Variables|Default|GetHitbox))
  (Variables|Default|SetStartPoint (Transformation|GetActorLocation))
  (bind _output_get (Variables|Default|SetEndPoint (Transformation|GetWorldLocation (Variables|Default|GetMoveTo))))
  (Variables|Default|SetCurrentTarget _output_get)
  (Variables|Default|SetInitial%20Rotation _rotation)
  (Variables|Default|SetInital%20Scale _scale)
  (Variables|Default|SetInitial%20Capsule%20Rotation (.Rotation (Math|Transform|BreakTransform (Transformation|GetRelativeTransform (Variables|Default|GetCapsuleComponent))))))

(event EventTick
  (params (DeltaSeconds :type Float%20%28single-precision%29))
  (bind _mesh (Variables|Character|GetMesh))
  (bind _returnvalue (Transformation|GetRelativeTransform _mesh))
  (bind _rotation (Math|Transform|BreakTransform _returnvalue))
  (bind (_roll _pitch _yaw) (Math|Rotator|BreakRotator _rotation))
  (if (not (Variables|Default|GetisDying))
    (Transformation|AddActorWorldOffset (* (Math|Vector|Normalize (- (Variables|Default|GetCurrentTarget) (Transformation|GetActorLocation))) (* (Variables|Default|GetMove%20Speed) (Utilities|Time|GetWorldDeltaSeconds))))
    (if (Variables|Default|GetMovingToEnd)
      (if (Math|Vector|Equal(Vector) (Variables|Default|GetEndPoint) (Transformation|GetActorLocation) 1e+01)
        (Variables|Default|SetMovingToEnd false)
        (Variables|Default|SetCurrentTarget (Variables|Default|GetStartPoint))
        (if (Variables|Default|GetRotateMeshAfterReachingEndPoint) :!label _label
          (Transformation|SetRelativeRotation (Variables|Character|GetMesh) (Math|Rotator|MakeRotator _roll _pitch (+ _yaw 1.8e+02)) false false)))
      (elif (Math|Vector|Equal(Vector) (Variables|Default|GetStartPoint) (Transformation|GetActorLocation) 1e+01)
        (Variables|Default|SetMovingToEnd true)
        (Variables|Default|SetCurrentTarget (Variables|Default|GetEndPoint))
        (goto _label)))))

(fn ConstructionScript
  (|CallParentFunction))