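; Quest actor for killing every Rhynoc in Mermaid Coast, with completion saved as a level bool.
; If already completed, BeginPlay destroys Sammy; otherwise it moves fairy Anna far away and binds to each enemy's killed event.
; Each kill triggers a delayed check of all enemy states.
; Once none remain alive, it moves Anna's ice block to her original spot, saves completion and teleports Sammy to start a conversation with the player.
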(event Custom|Enemy%20Has%20Been%20Killed
  (Utilities|FlowControl|Delay 0.2)
  (bind _some_enemies_are_alive (CallFunction|AreSomeEnemiesAlive?))
  (if (not _some_enemies_are_alive)
    (Utilities|FlowControl|DoOnce false
      (:Completed
        (CallFunction|OnQuestCompletion)))))

(event Custom|Hide%20fairy
  (bind _fairy__anna__ref (Variables|Default|GetFairy%20%28Anna%29%20Ref))
  (Variables|Default|SetInitial%20Fairy%20Location (Transformation|GetActorLocation _fairy__anna__ref))
  (Transformation|SetActorLocation _fairy__anna__ref "110000.000000, 0, 0" false false))

(event Custom|Unhide%20fairy
  (bind _outactors (Actor|GetAllActorsOfClass "/Game/SpyroContent/Global_Assets/Global_Level_Items/Dragon_Breath/Blueprints/Ice_Block/Blueprints/Ice_Block_BP.Ice_Block_BP_C"))
  (for _array_element _outactors
    (if (== (Variables|/Game/SpyroContent/Global_Assets/Global_Level_Items/Dragon_Breath/Blueprints/Ice_Block/Blueprints/Ice_Block_BP.Ice_Block_BP_C|GetFrozen_Character _array_element) (Variables|Default|GetFairy%20%28Anna%29%20Ref))
      (Transformation|SetActorLocation _array_element (Variables|Default|GetInitial%20Fairy%20Location) false false))))

(event Custom|On%20Quest%20Completion
  (bind _sammy_teleport_point (Variables|Default|GetSammy%20teleport%20point))
  (bind _returnvalue (Transformation|GetWorldTransform _sammy_teleport_point))
  (CallFunction|UnhideFairy)
  (CallFunction|SetLevelBool (Variables|Default|GetCurrent%20Level%20Name) (Variables|Default|GetLevel%20Bool%20ID) self (Class|KismetSystemLibrary|MakeLiteralBool true))
  (Transformation|SetActorLocationAndRotation (Variables|Default|GetSammy%20Ref) (.location _returnvalue) (.rotation _returnvalue) false true)
  (bind _returnvalue_2 (Actor|GetActorOfClass "/Game/SpyroContent/Global_Assets/Global_Characters/Playable_Characters/BP_Base_Playable.BP_Base_Playable_C"))
  (Default|TeleporttoTalktoMe (Variables|Default|GetSammy%20Ref) _returnvalue_2 0.5))

(event Custom|On%20Begin%20Play%20If%20Quest%20NOT%20Completed
  (CallFunction|HideFairy)
  (bind _outactors (Actor|GetAllActorsOfClass "/Game/SpyroContent/Global_Assets/Global_Characters/AI_Characters/Actors/Enemies/Base_Enemy_BP.Base_Enemy_BP_C"))
  (for _array_element _outactors
    (EventDispatchers|BindEventtoIWasKilledandLaunched (Variables|/Game/SpyroContent/Global_Assets/Global_Characters/AI_Characters/Actors/Base_AICharacter_BP.Base_AICharacter_BP_C|GetWalking_AI_Character _array_element) (delegate Custom|Enemy%20Has%20Been%20Killed))))

(event Custom|On%20Begin%20Play%20If%20Quest%20IS%20Already%20Completed
  (Actor|DestroyActor (Variables|Default|GetSammy%20Ref)))

(event EventBeginPlay
  (bind _returnvalue (CallFunction|GetLevelBools (Variables|Default|GetCurrent%20Level%20Name) self))
  (if (Utilities|Array|Get(acopy) _returnvalue (Variables|Default|GetLevel%20Bool%20ID))
    (CallFunction|OnBeginPlayifQuestISAlreadyCompleted)
    (else
      (CallFunction|OnBeginPlayifQuestNOTCompleted))))

(fn ConstructionScript)

(fn AreSomeEnemiesAlive?
  (LocalVariables|SetSome%20are%20alive false)
  (bind _outactors (Actor|GetAllActorsOfClass "/Game/SpyroContent/Global_Assets/Global_Characters/AI_Characters/Actors/Enemies/Base_Enemy_BP.Base_Enemy_BP_C"))
  (bind _array_element (Utilities|Array|ForEachLoopwithBreak _outactors :!label _label)
    (:LoopBody
      (if (not (Utilities|Enum|Equal(Enum) (Variables|/Game/SpyroContent/Global_Assets/Global_Components/Base_AI_Character.Base_AI_Character_C|GetAICharacter_State (Variables|/Game/SpyroContent/Global_Assets/Global_Characters/AI_Characters/Actors/Base_AICharacter_BP.Base_AICharacter_BP_C|GetWalking_AI_Character _array_element)) "NewEnumerator3"))
        (LocalVariables|SetSome%20are%20alive true)
        (goto _label Break)))
    (:Completed
      (return (LocalVariables|GetSome%20are%20alive)))))