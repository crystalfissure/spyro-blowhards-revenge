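; BP_Pumpkin is a Spyro quest pumpkin, derived from a treasure container, that lights up when hit by a specific damage type.
; Lighting swaps its mesh and material, shows the drop shadow, plays a sound and fires a dispatcher.
; It scans all pumpkins to count lit ones for the quest HUD, refreshed on container reset.
; When successfully damaged as a container, it also flags whether it is the last pumpkin lit.
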(event Custom|Lit%20the%20pumpkin%20up
  (Components|StaticMesh|SetStaticMesh (Variables|Default|GetStaticMesh) (Variables|Default|GetLit%20up%20pumpkin%20static%20mesh))
  (Rendering|Material|SetMaterial (Variables|Default|GetStaticMesh) 0 (Variables|Default|GetLit%20up%20pumpkin%20material))
  (Rendering|SetVisibility (Variables|Default|GetDropshadow) true false)
  (Variables|Default|SetIs%20lit%20up true)
  (Default|CallIHaveBeenLitUp!))

(event Custom|On%20Damage%20Dealt
  (if (Utilities|Enum|Equal(Enum) (Variables|/Game/SpyroContent/Global_Assets/Global_Components/Damageable_Com.Damageable_Com_C|GetDeal%20Damage%20-%20Damage%20Type (Variables|Default|GetDamageable)) "NewEnumerator1")
    (if (not (Variables|Default|GetIs%20lit%20up))
      (Audio|PlaySoundatLocation (Variables|Default|GetPumpkin%20lit%20up%20SFX) (Transformation|GetActorLocation) "0, 0,0.000000" 2.0 0.8 0.0 "/Game/SpyroContent/Global_Assets/Global_Audio/Attenuation/Spyro_Attenuation_MediumHigh.Spyro_Attenuation_MediumHigh" 0 0)
      (CallFunction|LitthePumpkinUp)
      (bind _asspyro_player_controller (Utilities|Casting|CastToSpyro_PlayerController (Game|GetPlayerController 0)))
      (bind _total_number_destroyed (CallFunction|CountPumpkins))
      (Default|ShowBottomRightQuestHUD _asspyro_player_controller (Variables|Default|GetPumpkin%20HUD%20sprite) (Utilities|String|ToString(Integer) _total_number_destroyed) (Variables|Default|GetTotal%20number%20of%20pumpkins)))))

(event EventResetThisContainer
  (|CallParentFunction)
  (bind _asspyro_player_controller (Utilities|Casting|CastToSpyro_PlayerController (Game|GetPlayerController 0)))
  (bind _total_number_destroyed (CallFunction|CountPumpkins))
  (Rendering|Components|TextRender|SetText (Variables|/Game/SpyroContent/Global_Assets/Global_UserInterface/Widgets/HUD.HUD_C|GetQuestItem_TextBlock_BottomRight (Variables|/Game/SpyroContent/Global_Assets/Global_Characters/Playable_Characters/Spyro_PlayerController.Spyro_PlayerController_C|GetMy_HUD_Ref _asspyro_player_controller)) (Utilities|Text|ToText(String) (Utilities|String|Append (Utilities|String|ToString(Integer) _total_number_destroyed) "/" (Variables|Default|GetTotal%20number%20of%20pumpkins)))))

(event EventBeginPlay
  (|CallParentFunction)
  (EventDispatchers|BindEventtoCallDealDamage (Variables|Default|GetDamageable) (delegate Custom|On%20Damage%20Dealt)))

(event EventTreasureContainerSuccessfullyDamaged
  (|CallParentFunction)
  (Variables|Default|SetIm_The_Last_Pumpkin_Lit_Up true)
  (bind _outactors (Actor|GetAllActorsOfClass "BP_Pumpkin_C"))
  (for _array_element _outactors
    (if (and (not (== _array_element self)) (not (Variables|BP_Pumpkin_C|GetIs%20lit%20up _array_element)))
      (Variables|Default|SetIm_The_Last_Pumpkin_Lit_Up false))))

(fn ConstructionScript
  (|CallParentFunction))

(fn CountPumpkins
  (LocalVariables|Setnumber%20destroyed 0)
  (bind _outactors (Actor|GetAllActorsOfClass "BP_Pumpkin_C"))
  (for _array_element _outactors
    (if (Variables|BP_Pumpkin_C|GetIs%20lit%20up _array_element)
      (Math|Integer|IncrementInt (LocalVariables|Getnumber%20destroyed))))
  (return (LocalVariables|Getnumber%20destroyed)))