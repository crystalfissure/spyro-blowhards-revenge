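; Level quest manager for lighting every BP_Pumpkin to reveal a fairy in the Spyro remake.
; If the saved level bool shows completion, all pumpkins start lit; otherwise it moves the fairy far away and listens for each pumpkin lighting.
; Once the lit count reaches the total, it saves completion, moves the ice block holding the fairy to the fairy's original location and hides the quest HUD.
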(event Custom|Pumpkin%20has%20been%20lit%20up
  (Utilities|FlowControl|Delay 0.2)
  (bind _total_number_lit_up (CallFunction|CountPumpkins))
  (if (== _total_number_lit_up (Variables|Default|GetTotal%20number%20of%20pumpkins))
    (CallFunction|SetLevelBool (Variables|Default|GetCurrent%20Level%20Name) (Variables|Default|GetLevel%20Quest%20ID) self (Class|KismetSystemLibrary|MakeLiteralBool true))
    (CallFunction|UnhideFairy)
    (bind _asspyro_player_controller (Utilities|Casting|CastToSpyro_PlayerController (Game|GetPlayerController 0)))
    (Default|HideBottomRightQuestHUD _asspyro_player_controller)))

(event Custom|Hide%20fairy
  (bind _fairy_ref (Variables|Default|GetFairy%20Ref))
  (Variables|Default|SetInitial%20Fairy%20Location (Transformation|GetActorLocation _fairy_ref))
  (Transformation|SetActorLocation _fairy_ref "100000.000000, 0, 0" false false))

(event Custom|Unhide%20fairy
  (bind _outactors (Actor|GetAllActorsOfClass "/Game/SpyroContent/Global_Assets/Global_Level_Items/Dragon_Breath/Blueprints/Ice_Block/Blueprints/Ice_Block_BP.Ice_Block_BP_C"))
  (for _array_element _outactors
    (if (== (Variables|/Game/SpyroContent/Global_Assets/Global_Level_Items/Dragon_Breath/Blueprints/Ice_Block/Blueprints/Ice_Block_BP.Ice_Block_BP_C|GetFrozen_Character _array_element) (Variables|Default|GetFairy%20Ref))
      (Transformation|SetActorLocation _array_element (Variables|Default|GetInitial%20Fairy%20Location) false false))))

(event EventBeginPlay
  (bind _outactors (Actor|GetAllActorsOfClass "/Game/Remakes/SoI/Quests/Pumpkins/BP_Pumpkin.BP_Pumpkin_C"))
  (Variables|Default|SetPumpkins _outactors)
  (bind _returnvalue (CallFunction|GetLevelBools (Variables|Default|GetCurrent%20Level%20Name) self))
  (if (Utilities|Array|Get(acopy) _returnvalue (Variables|Default|GetLevel%20Quest%20ID))
    (for _array_element (Variables|Default|GetPumpkins)
      (Default|LitthePumpkinUp _array_element))
    (else
      (CallFunction|HideFairy)
      (for _array_element_2 (Variables|Default|GetPumpkins)
        (EventDispatchers|BindEventtoIHaveBeenLitUp! _array_element_2 (delegate Custom|Pumpkin%20has%20been%20lit%20up))))))

(event Collision|EventActorBeginOverlap
  (params (OtherActor :type Actor%20Object%20Reference)))

(event EventTick
  (params (DeltaSeconds :type Float%20%28single-precision%29)))

(fn ConstructionScript)

(fn CountPumpkins
  (LocalVariables|Setnumber%20destroyed 0)
  (bind _outactors (Actor|GetAllActorsOfClass "/Game/Remakes/SoI/Quests/Pumpkins/BP_Pumpkin.BP_Pumpkin_C"))
  (for _array_element _outactors
    (if (Variables|/Game/Remakes/SoI/Quests/Pumpkins/BP_Pumpkin.BP_Pumpkin_C|GetIs%20lit%20up _array_element)
      (Math|Integer|IncrementInt (LocalVariables|Getnumber%20destroyed))))
  (return (LocalVariables|Getnumber%20destroyed)))