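; Sandcastle-smashing quest actor that tracks destroyed Sandcastle_BP actors and saves completion as a per-level bool.
; If already completed, BeginPlay swaps castles for destroyed versions; otherwise it moves the fairy to an upward holding spot and binds to each castle's damage event.
; Each hit recounts and updates the quest HUD.
; When all fall, it saves, returns the fairy and any Ice_Block_BP freezing it, hides the HUD and stops castle drop respawns.
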(event Custom|Sandcastle%20Has%20Been%20Destroyed
  (Utilities|FlowControl|Delay 0.2)
  (bind _asspyro_player_controller (Utilities|Casting|CastToSpyro_PlayerController (Game|GetPlayerController 0)))
  (bind _total_destroyed (CallFunction|CountSandcastles))
  (Default|ShowBottomLeftQuestHUD _asspyro_player_controller (Variables|Default|GetSandcastle%20HUD%20sprite) (Utilities|String|ToString(Integer) _total_destroyed) (Utilities|String|ToString(Integer) (Variables|Default|GetTotal%20number%20of%20sandcastles)))
  (if (== _total_destroyed (Variables|Default|GetTotal%20number%20of%20sandcastles))
    (Utilities|FlowControl|DoOnce false
      (:Completed
        (CallFunction|OnQuestCompletion)))))

(event Custom|On%20Begin%20Play%20If%20Quest%20NOT%20Completed
  (CallFunction|TeleportFairytoUpwardLocation)
  (for _array_element (Variables|Default|GetSandcastles)
    (EventDispatchers|BindEventtoContainerSuccessfullyDamaged _array_element (delegate Custom|Sandcastle%20Has%20Been%20Destroyed))))

(event Custom|On%20Begin%20Play%20If%20Quest%20IS%20Already%20Completed
  (for _array_element (Variables|Default|GetSandcastles)
    (Game|SpawnActorfromClass "/Game/Remakes/SoI/Quests/Sandcastles/Assets/BP_Destroyed_Sandcastle.BP_Destroyed_Sandcastle_C" (Transformation|GetActorTransform _array_element) "Undefined" 0 0)
    (Actor|DestroyActor _array_element)))

(event Custom|On%20Quest%20Completion
  (CallFunction|SetLevelBool (Variables|Default|GetCurrent%20Level%20Name) (Variables|Default|GetLevel%20Bool%20ID) self (Class|KismetSystemLibrary|MakeLiteralBool true))
  (CallFunction|TeleportFairytoInitialLocation)
  (bind _asspyro_player_controller (Utilities|Casting|CastToSpyro_PlayerController (Game|GetPlayerController 0)))
  (Default|HideBottomLeftQuestHUD _asspyro_player_controller)
  (for _array_element (Variables|Default|GetSandcastles)
    (Variables|/Game/SpyroContent/Global_Assets/Global_Components/Drops_Items.Drops_Items_C|Setnever%20respawn (Variables|/Game/SpyroContent/Global_Assets/Global_Level_Items/Treasure_Containers/Treasure_Container_Base_BP.Treasure_Container_Base_BP_C|GetItem_Drop_Component _array_element) true)))

(event Custom|Teleport%20fairy%20to%20initial%20location
  (bind _initial_fairy_location (Variables|Default|GetInitial%20Fairy%20Location))
  (bind _outactors (Actor|GetAllActorsOfClass "/Game/SpyroContent/Global_Assets/Global_Level_Items/Dragon_Breath/Blueprints/Ice_Block/Blueprints/Ice_Block_BP.Ice_Block_BP_C"))
  (for _array_element _outactors
    (if (== (Variables|/Game/SpyroContent/Global_Assets/Global_Level_Items/Dragon_Breath/Blueprints/Ice_Block/Blueprints/Ice_Block_BP.Ice_Block_BP_C|GetFrozen_Character _array_element) (Variables|Default|GetFairy%20Ref))
      (Transformation|SetActorLocation _array_element _initial_fairy_location false false)))
  (Transformation|SetActorLocation (Variables|Default|GetFairy%20Ref) _initial_fairy_location false false))

(event Custom|Teleport%20fairy%20to%20upward%20location
  (bind _fairy_ref (Variables|Default|GetFairy%20Ref))
  (Variables|Default|SetInitial%20Fairy%20Location (Transformation|GetActorLocation _fairy_ref))
  (Transformation|SetActorLocation _fairy_ref (Transformation|GetWorldLocation (Variables|Default|GetFairy%20Location%20While%20Sandcastles%20Are%20Intact)) false false))

(event EventBeginPlay
  (bind _outactors (Actor|GetAllActorsOfClass "/Game/Remakes/SoI/Quests/Sandcastles/Sandcastle_BP.Sandcastle_BP_C"))
  (Variables|Default|SetSandcastles _outactors)
  (bind _returnvalue (CallFunction|GetLevelBools (Variables|Default|GetCurrent%20Level%20Name) self))
  (if (Utilities|Array|Get(acopy) _returnvalue (Variables|Default|GetLevel%20Bool%20ID))
    (CallFunction|OnBeginPlayifQuestISAlreadyCompleted)
    (else
      (CallFunction|OnBeginPlayifQuestNOTCompleted))))

(fn ConstructionScript)

(fn CountSandcastles
  (LocalVariables|SetTotal%20of%20destroyed 0)
  (bind _outactors (Actor|GetAllActorsOfClass "/Game/Remakes/SoI/Quests/Sandcastles/Sandcastle_BP.Sandcastle_BP_C"))
  (for _array_element _outactors
    (if (Variables|/Game/SpyroContent/Global_Assets/Global_Level_Items/Treasure_Containers/Treasure_Container_Base_BP.Treasure_Container_Base_BP_C|GetContainer_Destroyed _array_element)
      (Math|Integer|IncrementInt (LocalVariables|GetTotal%20of%20destroyed))))
  (return (LocalVariables|GetTotal%20of%20destroyed)))