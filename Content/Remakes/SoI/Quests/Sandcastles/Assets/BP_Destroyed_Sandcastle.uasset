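; Destroyed sandcastle for the sandcastles quest that animates its collapse through a skeletal mesh morph target.
; On BeginPlay it applies the AnimPlayRate variable to both timelines through the SetAnimPlayrate event.
; The Linear flag then picks which timeline plays from start, and that timeline's track drives the "Key 1" morph weight on each update.
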(event Custom|Set%20Anim%20Playrate
  (params (Play%20Rate :type Float%20%28single-precision%29))
  (Components|Timeline|SetPlayRate (Variables|Default|GetTimeline_0) Play%20Rate)
  (Components|Timeline|SetPlayRate (Variables|Default|GetTimeline_1) Play%20Rate))

(event EventBeginPlay
  (bind _skeletalmesh (Variables|Default|GetSkeletalMesh))
  (CallFunction|SetAnimPlayrate (Variables|Default|GetAnim%20Play%20Rate))
  (if (Variables|Default|GetLinear)
    (bind _newtrack_0 (Timeline|Timeline_0 PlayFromStart)
      (:Update
        (Components|SkeletalMesh|SetMorphTarget _skeletalmesh "Key 1" _newtrack_0 true)))
    (else
      (bind _newtrack_0_2 (Timeline|Timeline_1 PlayFromStart)
        (:Update
          (Components|SkeletalMesh|SetMorphTarget _skeletalmesh "Key 1" _newtrack_0_2 true))))))

(fn ConstructionScript)