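; Level quest manager that tracks lit lighthouses and rewards lighting them all by bringing back the frozen fairy Rachel.
; BeginPlay checks a saved level bool, then either restores the completed state or hides Rachel off-map and binds to each lighthouse's lit event.
; Each lighting updates the quest HUD count.
; Completion moves Rachel's ice block back, saves the bool, and chains Stanley and Stacey's new dialogue through teleport and autotalk.
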(event Custom|Lighthouse%20Has%20Been%20Lit%20Up
  (bind _total_number_of_lighthouses (Variables|Default|GetTotal%20number%20of%20lighthouses))
  (Utilities|FlowControl|Delay 0.2)
  (bind _asspyro_player_controller (Utilities|Casting|CastToSpyro_PlayerController (Game|GetPlayerController 0)))
  (bind _total_destroyed (CallFunction|CountLighthouses))
  (Default|ShowBottomRightQuestHUD _asspyro_player_controller (Variables|Default|GetLighthouse%20HUD%20sprite) (Utilities|String|ToString(Integer) _total_destroyed) (Utilities|String|ToString(Integer) _total_number_of_lighthouses))
  (if (== _total_destroyed _total_number_of_lighthouses)
    (Utilities|FlowControl|DoOnce false
      (:Completed
        (CallFunction|OnQuestCompletion)))))

(event Custom|Hide%20fairy
  (bind _fairy__rachel__ref (Variables|Default|GetFairy%20%28Rachel%29%20Ref))
  (Variables|Default|SetInitial%20Fairy%20Location (Transformation|GetActorLocation _fairy__rachel__ref))
  (Transformation|SetActorLocation _fairy__rachel__ref "100000.000000, 0, 0" false false))

(event Custom|Unhide%20fairy
  (bind _outactors (Actor|GetAllActorsOfClass "/Game/SpyroContent/Global_Assets/Global_Level_Items/Dragon_Breath/Blueprints/Ice_Block/Blueprints/Ice_Block_BP.Ice_Block_BP_C"))
  (for _array_element _outactors
    (if (== (Variables|/Game/SpyroContent/Global_Assets/Global_Level_Items/Dragon_Breath/Blueprints/Ice_Block/Blueprints/Ice_Block_BP.Ice_Block_BP_C|GetFrozen_Character _array_element) (Variables|Default|GetFairy%20%28Rachel%29%20Ref))
      (Transformation|SetActorLocation _array_element (Variables|Default|GetInitial%20Fairy%20Location) false false))))

(event Custom|On%20Quest%20Completion
  (bind _stacey_teleport_point (Variables|Default|GetStacey%20teleport%20point))
  (bind _stacey_ref (Variables|Default|GetStacey%20Ref))
  (bind _stanley_ref (Variables|Default|GetStanley%20Ref))
  (bind _returnvalue (Transformation|GetWorldTransform _stacey_teleport_point))
  (CallFunction|UnhideFairy)
  (CallFunction|SetLevelBool (Variables|Default|GetCurrent%20Level%20Name) (Variables|Default|GetLevel%20Bool%20ID) self (Class|KismetSystemLibrary|MakeLiteralBool true))
  (bind _asspyro_player_controller (Utilities|Casting|CastToSpyro_PlayerController (Game|GetPlayerController 0)))
  (Default|HideBottomRightQuestHUD _asspyro_player_controller)
  (Variables|/Game/SpyroContent/Global_Assets/Global_Characters/NPCs/NPC_Base_BP.NPC_Base_BP_C|SetDialogue_Info _stanley_ref (Variables|Default|GetStanley%20dialogue%20after%20completing%20quest))
  (EventDispatchers|BindEventtoDoneTalking _stanley_ref (delegate Custom|Autotalk%20after%20done%20talking%20to%20stanley))
  (Variables|/Game/SpyroContent/Global_Assets/Global_Characters/NPCs/NPC_Base_BP.NPC_Base_BP_C|SetTalk_Again_Dialogue_Info _stanley_ref (Variables|Default|GetStanley%20talk%20again%20dialogue%20after%20completing%20quest))
  (bind _returnvalue_2 (Actor|GetActorOfClass "/Game/SpyroContent/Global_Assets/Global_Characters/Playable_Characters/BP_Base_Playable.BP_Base_Playable_C"))
  (Default|TeleporttoTalktoMe _stanley_ref _returnvalue_2 0.5)
  (Transformation|SetActorLocationAndRotation (Variables|Default|GetStacey%20Ref) (.location _returnvalue) (.rotation _returnvalue) false true)
  (Variables|/Game/SpyroContent/Global_Assets/Global_Characters/NPCs/NPC_Base_BP.NPC_Base_BP_C|SetDialogue_Info _stacey_ref (Variables|Default|GetStacey%20dialogue%20after%20completing%20quest))
  (Variables|/Game/SpyroContent/Global_Assets/Global_Characters/NPCs/NPC_Base_BP.NPC_Base_BP_C|SetTalk_Again_Dialogue_Info _stacey_ref (Variables|Default|GetStacey%20talk%20again%20dialogue%20after%20completing%20quest))
  (Utilities|FlowControl|Delay 1.0)
  (Variables|/Game/SpyroContent/Global_Assets/Global_Characters/NPCs/NPC_Base_BP.NPC_Base_BP_C|SetAutotalks (Variables|Default|GetStacey%20Ref) true))

(event Custom|Autotalk%20after%20done%20talking%20to%20stanley
  (Utilities|FlowControl|DoOnce false
    (:Completed
      (Utilities|FlowControl|Delay 0.1)
      (bind _returnvalue (Actor|GetActorOfClass "/Game/SpyroContent/Global_Assets/Global_Characters/Playable_Characters/BP_Base_Playable.BP_Base_Playable_C"))
      (Default|Autotalk? (Variables|Default|GetStacey%20Ref) _returnvalue (Variables|/Script/Engine.Character|GetCapsuleComponent _returnvalue) true))))

(event Custom|On%20Begin%20Play%20If%20Quest%20NOT%20Completed
  (CallFunction|HideFairy)
  (for _array_element (Variables|Default|GetLighthouses)
    (EventDispatchers|BindEventtoIHaveBeenLitUp! _array_element (delegate Custom|Lighthouse%20Has%20Been%20Lit%20Up))))

(event Custom|On%20Begin%20Play%20If%20Quest%20IS%20Already%20Completed
  (Actor|DestroyActor (Variables|Default|GetStanley%20Ref))
  (for _array_element (Variables|Default|GetLighthouses)
    (Default|LittheLighthouseUp _array_element)))

(event EventBeginPlay
  (bind _outactors (Actor|GetAllActorsOfClass "/Game/Remakes/SoI/Quests/Lighthouses/BP_Lighthouse.BP_Lighthouse_C"))
  (Variables|Default|SetLighthouses _outactors)
  (bind _returnvalue (CallFunction|GetLevelBools (Variables|Default|GetCurrent%20Level%20Name) self))
  (if (Utilities|Array|Get(acopy) _returnvalue (Variables|Default|GetLevel%20Bool%20ID))
    (CallFunction|OnBeginPlayifQuestISAlreadyCompleted)
    (else
      (CallFunction|OnBeginPlayifQuestNOTCompleted))))

(fn ConstructionScript)

(fn CountLighthouses
  (LocalVariables|SetTotal%20of%20destroyed 0)
  (bind _outactors (Actor|GetAllActorsOfClass "/Game/Remakes/SoI/Quests/Lighthouses/BP_Lighthouse.BP_Lighthouse_C"))
  (for _array_element _outactors
    (if (Variables|/Game/Remakes/SoI/Quests/Lighthouses/BP_Lighthouse.BP_Lighthouse_C|GetIs%20lit%20up _array_element)
      (Math|Integer|IncrementInt (LocalVariables|GetTotal%20of%20destroyed))))
  (return (LocalVariables|GetTotal%20of%20destroyed)))