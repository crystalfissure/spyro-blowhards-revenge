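; BP_Lighthouse is a damageable lighthouse, built on a treasure container parent, that lights up when hit by a specific damage type.
; It binds to its Damageable component's damage event and, on the first matching hit while unlit, plays an attenuated sound.
; Lighting swaps the static mesh and material, sets IsLitUp and calls IHaveBeenLitUp to announce the change.
; The container's damaged and reset events simply pass through to the parent.
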(event Custom|Lit%20the%20lighthouse%20up
  (Components|StaticMesh|SetStaticMesh (Variables|Default|GetStaticMesh) (Variables|Default|GetLit%20up%20lighthouse%20static%20mesh))
  (Rendering|Material|SetMaterial (Variables|Default|GetStaticMesh) 0 (Variables|Default|GetLit%20up%20lighthouse%20material))
  (Variables|Default|SetIs%20lit%20up true)
  (Default|CallIHaveBeenLitUp!))

(event Custom|On%20Damage%20Dealt
  (if (Utilities|Enum|Equal(Enum) (Variables|/Game/SpyroContent/Global_Assets/Global_Components/Damageable_Com.Damageable_Com_C|GetDeal%20Damage%20-%20Damage%20Type (Variables|Default|GetDamageable)) "NewEnumerator1")
    (if (not (Variables|Default|GetIs%20lit%20up))
      (Audio|PlaySoundatLocation (Variables|Default|GetLighthouse%20lit%20up%20SFX) (Transformation|GetActorLocation) "0, 0, 0" 2.0 0.8 0.0 "/Game/SpyroContent/Global_Assets/Global_Audio/Attenuation/Spyro_Attenuation_MediumHigh.Spyro_Attenuation_MediumHigh" 0 0)
      (CallFunction|LittheLighthouseUp))))

(event EventResetThisContainer
  (|CallParentFunction))

(event EventBeginPlay
  (|CallParentFunction)
  (EventDispatchers|BindEventtoCallDealDamage (Variables|Default|GetDamageable) (delegate Custom|On%20Damage%20Dealt)))

(event EventTreasureContainerSuccessfullyDamaged
  (|CallParentFunction))

(fn ConstructionScript
  (|CallParentFunction))