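; Collectible fairy NPC that starts frozen in ice and awards a saved collectible, with burst effect and sound, when thawed.
; BeginPlay colors the fairy through dynamic materials, freezes it and cancels the block's melt timer, optionally making it fire-only.
; The thaw callback runs the award once.
; As a workaround for leftover blocks on level travel, portal overlap or destruction melts the block, with portal overlap suppressing the award.
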(event Custom|Fairy%20melted
  (bind _vfx_spawn_point (Variables|Default|GetVFX%20Spawn%20Point))
  (bind _returnvalue (Transformation|GetWorldLocation _vfx_spawn_point))
  (if (not (Variables|Default|GetPlayer%20overlapped%20portal))
    (Utilities|FlowControl|DoOnce false
      (:Completed
        (Variables|Default|SetWon't%20Talk (Variables|Default|GetWon't%20Talk%20After%20Thawing))
        (bind _asspyro_persistant_data (Utilities|Casting|CastToSpyro_PersistantData (Game|GetGameInstance)))
        (if (Variables|Default|GetDEBUG%20Don't%20Save%20a%20collectible)
          _
          (else
            (Default|SaveACollectible _asspyro_persistant_data (Variables|Default|GetType%20Of%20Collectable) "" (Variables|Default|GetHUD%20Update%20Delay) (Variables|/Game/SpyroContent/Global_Assets/Global_Components/NPC_Award_Item.NPC_Award_Item_C|GetLevel%20Item%20Index (Variables|Default|GetNPC_Award_Item)) (Variables|Default|GetSkill%20Award))
            (if (Utilities|Enum|Equal(Enum) (Variables|Default|GetType%20Of%20Collectable) "NewEnumerator1")
              (bind _asspyro_player_controller (Utilities|Casting|CastToSpyro_PlayerController (Game|GetPlayerController 0)))
              (Default|ShowPrimaryCollectibleHUD _asspyro_player_controller 3.0))))
        (Effects|SpawnEmitteratLocation "/Game/SpyroContent/Global_Assets/Global_Level_Items/Treasure_Containers/Mystery_Vase/Myster_Vase_Burst.Myster_Vase_Burst" _returnvalue)
        (Audio|PlaySoundatLocation "/Game/Remakes/SoI/Collectibles/Fairy/Assets/Fairy_Collected.Fairy_Collected" _returnvalue "0, 0, 0" 1.0 1.0 0.0 0 0 0)))))

(event Custom|Customize%20looks
  (bind _mesh (Variables|Character|GetMesh))
  (bind _mesh_2 (Variables|Character|GetMesh))
  (bind _appearance (Variables|Default|GetAppearance))
  (bind (_skincolor _skinbrightness _wingscolor _wingsbrightness _dresscolor _dressbrightness _lipcolor _lipbrightness _eyecolor _eyebrightness _eyebrowscolor _eyebrowsbrightness _bigponytail _haircolor _hairbrightness) (Utilities|Struct|BreakFairy_Appearance _appearance))
  (Utilities|FlowControl|Sequence
    (:then_0
      ;[0 0 0] Dragon wings off
      (Rendering|Material|SetMaterial (Variables|Character|GetMesh) 3 "/Game/SpyroContent/Global_Assets/Global_Materials/Material_Instances/Invisible_Mat.Invisible_Mat")
      ;[0 0 0] Helmet off
      (Rendering|Material|SetMaterial (Variables|Character|GetMesh) 12 "/Game/SpyroContent/Global_Assets/Global_Materials/Material_Instances/Invisible_Mat.Invisible_Mat")
      ;[0 0 0] Shield off
      (Rendering|Material|SetMaterial (Variables|Character|GetMesh) 5 "/Game/SpyroContent/Global_Assets/Global_Materials/Material_Instances/Invisible_Mat.Invisible_Mat")
      ;[0 0 0] Infinity symbol off
      (Rendering|Material|SetMaterial (Variables|Character|GetMesh) 2 "/Game/SpyroContent/Global_Assets/Global_Materials/Material_Instances/Invisible_Mat.Invisible_Mat")
      ;[0 0 0] Dress overlap for super fairies (off)
      (Rendering|Material|SetMaterial (Variables|Character|GetMesh) 13 "/Game/SpyroContent/Global_Assets/Global_Materials/Material_Instances/Invisible_Mat.Invisible_Mat"))
    (:then_1
      ;[0 0 0] Skin color
      (bind _returnvalue (Rendering|Material|CreateDynamicMaterialInstance (Variables|Character|GetMesh) 6 "/Game/SpyroContent/Global_Assets/Global_Materials/Material_Instances/Untex_Vertex_Color.Untex_Vertex_Color" "None" :!class /Script/Engine.PrimitiveComponent))
      (Rendering|Material|SetVectorParameterValue _returnvalue "ColorChange" _skincolor :!class /Script/Engine.MaterialInstanceDynamic)
      (Rendering|Material|SetScalarParameterValue _returnvalue "Brightness" _skinbrightness :!class /Script/Engine.MaterialInstanceDynamic))
    (:then_2
      ;[0 0 0] Wings color
      (bind _returnvalue_2 (Rendering|Material|CreateDynamicMaterialInstance (Variables|Character|GetMesh) 4 "/Game/SpyroContent/Global_Assets/Global_Materials/Material_Instances/Untex_Vertex_Color_2Sided.Untex_Vertex_Color_2Sided" "None" :!class /Script/Engine.PrimitiveComponent))
      (Rendering|Material|SetVectorParameterValue _returnvalue_2 "ColorChange" _wingscolor :!class /Script/Engine.MaterialInstanceDynamic)
      (Rendering|Material|SetScalarParameterValue _returnvalue_2 "Opacity" 0.3 :!class /Script/Engine.MaterialInstanceDynamic)
      (Rendering|Material|SetScalarParameterValue _returnvalue_2 "Brightness" _wingsbrightness :!class /Script/Engine.MaterialInstanceDynamic))
    (:then_3
      ;[0 0 0] Dress color
      (bind _returnvalue_3 (Rendering|Material|CreateDynamicMaterialInstance (Variables|Character|GetMesh) 10 0 "None" :!class /Script/Engine.PrimitiveComponent))
      (Rendering|Material|SetVectorParameterValue _returnvalue_3 "ColorChange" _dresscolor :!class /Script/Engine.MaterialInstanceDynamic)
      (Rendering|Material|SetScalarParameterValue _returnvalue_3 "Brightness" _dressbrightness :!class /Script/Engine.MaterialInstanceDynamic))
    (:then_4
      ;[0 0 0] Lip color
      (bind _returnvalue_4 (Rendering|Material|CreateDynamicMaterialInstance (Variables|Character|GetMesh) 9 "/Game/SpyroContent/Global_Assets/Global_Materials/Material_Instances/Untex_Vertex_Color.Untex_Vertex_Color" "None" :!class /Script/Engine.PrimitiveComponent))
      (Rendering|Material|SetVectorParameterValue _returnvalue_4 "ColorChange" _lipcolor :!class /Script/Engine.MaterialInstanceDynamic)
      (Rendering|Material|SetScalarParameterValue _returnvalue_4 "Brightness" _lipbrightness :!class /Script/Engine.MaterialInstanceDynamic))
    (:then_5
      ;[0 0 0] Eye color
      (bind _returnvalue_5 (Rendering|Material|CreateDynamicMaterialInstance (Variables|Character|GetMesh) 7 "/Game/SpyroContent/Global_Assets/Global_Characters/NPCs/Fairies/Materials/Fairy_Eyes_Mat.Fairy_Eyes_Mat" "None" :!class /Script/Engine.PrimitiveComponent))
      (Rendering|Material|SetVectorParameterValue _returnvalue_5 "ColorChange" _eyecolor :!class /Script/Engine.MaterialInstanceDynamic)
      (Rendering|Material|SetScalarParameterValue _returnvalue_5 "Brightness" _eyebrightness :!class /Script/Engine.MaterialInstanceDynamic))
    (:then_6
      ;[0 0 0] Brows color
      (bind _returnvalue_6 (Rendering|Material|CreateDynamicMaterialInstance (Variables|Character|GetMesh) 11 "/Game/SpyroContent/Global_Assets/Global_Characters/NPCs/Fairies/Materials/Fairy_Eyes_Mat.Fairy_Eyes_Mat" "None" :!class /Script/Engine.PrimitiveComponent))
      (Rendering|Material|SetVectorParameterValue _returnvalue_6 "ColorChange" _eyebrowscolor :!class /Script/Engine.MaterialInstanceDynamic)
      (Rendering|Material|SetScalarParameterValue _returnvalue_6 "Brightness" _eyebrowsbrightness :!class /Script/Engine.MaterialInstanceDynamic))
    (:then_7
      ;[0 0 0] Hair color
      (if _bigponytail
        (Rendering|Material|SetMaterial _mesh 1 "/Game/SpyroContent/Global_Assets/Global_Materials/Material_Instances/Invisible_Mat.Invisible_Mat")
        (bind _returnvalue_7 (Rendering|Material|CreateDynamicMaterialInstance _mesh_2 0 "/Game/SpyroContent/Global_Assets/Global_Materials/Material_Instances/Untex_Vertex_Color.Untex_Vertex_Color" "None" :!class /Script/Engine.PrimitiveComponent))
        (Rendering|Material|SetVectorParameterValue _returnvalue_7 "ColorChange" _haircolor :!class /Script/Engine.MaterialInstanceDynamic)
        (Rendering|Material|SetScalarParameterValue _returnvalue_7 "Brightness" _hairbrightness :!class /Script/Engine.MaterialInstanceDynamic)
        (else
          (Rendering|Material|SetMaterial _mesh 0 "/Game/SpyroContent/Global_Assets/Global_Materials/Material_Instances/Invisible_Mat.Invisible_Mat")
          (bind _returnvalue_8 (Rendering|Material|CreateDynamicMaterialInstance _mesh_2 1 "/Game/SpyroContent/Global_Assets/Global_Materials/Material_Instances/Untex_Vertex_Color.Untex_Vertex_Color" "None" :!class /Script/Engine.PrimitiveComponent))
          (Rendering|Material|SetVectorParameterValue _returnvalue_8 "ColorChange" _haircolor :!class /Script/Engine.MaterialInstanceDynamic)
          (Rendering|Material|SetScalarParameterValue _returnvalue_8 "Brightness" _hairbrightness :!class /Script/Engine.MaterialInstanceDynamic)))
      (bind _returnvalue_9 (Rendering|Material|CreateDynamicMaterialInstance (Variables|Character|GetMesh) 8 "/Game/SpyroContent/Global_Assets/Global_Materials/Material_Instances/Untex_Vertex_Color.Untex_Vertex_Color" "None" :!class /Script/Engine.PrimitiveComponent))
      (Rendering|Material|SetVectorParameterValue _returnvalue_9 "ColorChange" _haircolor :!class /Script/Engine.MaterialInstanceDynamic)
      (Rendering|Material|SetScalarParameterValue _returnvalue_9 "Brightness" _hairbrightness :!class /Script/Engine.MaterialInstanceDynamic))))

(event Custom|Melt%20the%20ice%20block%20when%20player%20overlaps%20portal
  ;[0 0 0] The ice blocks weren't being melted when player traveled to other level so this janky workaround is needed
  (Variables|Default|SetPlayer%20overlapped%20portal true)
  (bind _outactors (Actor|GetAllActorsOfClass "/Game/SpyroContent/Global_Assets/Global_Level_Items/Dragon_Breath/Blueprints/Ice_Block/Blueprints/Ice_Block_BP.Ice_Block_BP_C"))
  (for _array_element _outactors
    (if (== (Variables|/Game/SpyroContent/Global_Assets/Global_Level_Items/Dragon_Breath/Blueprints/Ice_Block/Blueprints/Ice_Block_BP.Ice_Block_BP_C|GetFrozen_Character _array_element) self)
      (Default|Melt _array_element))))

(event EventBeginPlay
  (|CallParentFunction)
  (CallFunction|CustomizeLooks)
  (EventDispatchers|BindEventtoMeltedfromIce (Variables|Default|GetNPC_Damageable) (delegate Custom|Fairy%20melted))
  (Default|Freeze (Variables|Default|GetNPC_Damageable))
  ;[0 0 0] Prevent the fairy from melting after a few seconds
  (bind _outactors (Actor|GetAllActorsOfClass "/Game/SpyroContent/Global_Assets/Global_Level_Items/Dragon_Breath/Blueprints/Ice_Block/Blueprints/Ice_Block_BP.Ice_Block_BP_C"))
  (for _array_element _outactors
    (if (== (Variables|/Game/SpyroContent/Global_Assets/Global_Level_Items/Dragon_Breath/Blueprints/Ice_Block/Blueprints/Ice_Block_BP.Ice_Block_BP_C|GetFrozen_Character _array_element) self)
      (Utilities|Time|ClearTimerbyFunctionName _array_element "Melt Countdown")
      (if (Variables|Default|GetCan%20be%20freed%20only%20by%20flame%20attack)
        (Variables|/Game/SpyroContent/Global_Assets/Global_Components/Damageable_Com.Damageable_Com_C|SetDamage_Resistances (Variables|/Game/SpyroContent/Global_Assets/Global_Level_Items/Dragon_Breath/Blueprints/Ice_Block/Blueprints/Ice_Block_BP.Ice_Block_BP_C|GetDamageable _array_element) (Variables|Default|GetDamage%20Resistances%20-%20Fire%20Only)))))
  ;[0 0 0] The ice blocks weren't being melted when player traveled to other level so this janky workaround is needed
  (bind _outactors_2 (Actor|GetAllActorsOfClass "/Game/SpyroContent/Global_Assets/Global_Level_Items/Portals/Actors/BP_Portal.BP_Portal_C"))
  (for _array_element_2 _outactors_2
    (EventDispatchers|BindEventtoPlayerOverlappedMe _array_element_2 (delegate Custom|Melt%20the%20ice%20block%20when%20player%20overlaps%20portal))))

(event Collision|EventActorBeginOverlap
  (params (OtherActor :type Actor%20Object%20Reference))
  (|CallParentFunction OtherActor) ; This node is disabled and will not be called.\nDrag off pins to build functionality.
)

(event EventTick
  (params (DeltaSeconds :type Float%20%28single-precision%29))
  (|CallParentFunction DeltaSeconds) ; This node is disabled and will not be called.\nDrag off pins to build functionality.
)

(event EventDestroyed
  ;[0 0 0] Prevents a bug where if you re-entered the level, there would be ice blocks without fairy inside
  (bind _outactors (Actor|GetAllActorsOfClass "/Game/SpyroContent/Global_Assets/Global_Level_Items/Dragon_Breath/Blueprints/Ice_Block/Blueprints/Ice_Block_BP.Ice_Block_BP_C"))
  (for _array_element _outactors
    (if (== (Variables|/Game/SpyroContent/Global_Assets/Global_Level_Items/Dragon_Breath/Blueprints/Ice_Block/Blueprints/Ice_Block_BP.Ice_Block_BP_C|GetFrozen_Character _array_element) self)
      (Default|Melt _array_element))))

(fn ConstructionScript
  (|CallParentFunction))