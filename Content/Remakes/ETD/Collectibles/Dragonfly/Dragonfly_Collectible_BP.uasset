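; Dragonfly collectible that flees the player erratically within a wander radius of its spawn, returning home when no longer alerted.
; A moving bubble hitting its hitbox, or an NPC award, triggers a timeline capture animation.
; Afterwards it saves the collectible via the persistent game instance, or shows an already-owned widget if the save data has it.
; It then plays effects and destroys itself, first restoring player input and camera for NPC awards.
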(event OnComponentBeginOverlap(Hitbox)
  (params (OverlappedComponent :type Primitive%20Component%20Object%20Reference) (OtherActor :type Actor%20Object%20Reference) (OtherComp :type Primitive%20Component%20Object%20Reference) (OtherBodyIndex :type Integer) (bFromSweep :type Boolean) (SweepResult :type Hit%20Result%20Structure%20%28by%20ref%29))
  (bind _asbubble_moving_bp (Utilities|Casting|CastToBubble_Moving_BP OtherActor))
  (if (== (Variables|/Game/SpyroContent/Global_Assets/Global_Level_Items/Whirlwind/BP_Hurlwind.BP_Hurlwind_C|GetBox _asbubble_moving_bp) OtherComp)
    (Utilities|FlowControl|DoOnce false
      (:Completed
        (Actor|DestroyActor _asbubble_moving_bp)
        (CallFunction|CaptureSequence)))))

(event Custom|UpdateErraticAngle
  (Variables|Default|SetCurrentErraticAngle (Math|Random|RandomFloatinRange -6e+01 6e+01)))

(event Custom|Capture%20Sequence
  (bind _player_who_was_awarded_me (Variables|Default|GetPlayer%20Who%20Was%20Awarded%20Me))
  (bind _skeletalmesh (Variables|Default|GetSkeletalMesh))
  (bind _returnvalue (Transformation|GetWorldLocation _skeletalmesh))
  (bind _spyrocontr_ref (Variables|/Game/SpyroContent/Global_Assets/Global_Characters/Playable_Characters/BP_Base_Playable.BP_Base_Playable_C|GetSpyroContr_Ref _player_who_was_awarded_me))
  (Variables|Default|SetI%20was%20captured true)
  (Rendering|SetVisibility (Variables|Default|GetStaticMesh) true false)
  (bind (_direction _newtrack_0 _newtrack_1) (Timeline|Timeline_0 Play)
    (:Update
      (Transformation|SetRelativeLocationAndRotation (Variables|Default|GetSkeletalMesh) (Math|Vector|MakeVector 0.0 0.0 _newtrack_0) (Math|Rotator|MakeRotator 0.0 0.0 (+ _newtrack_1 -9e+01)) false false))
    (:Finished
      (bind _have_it_already_ (|CheckifWeAlreadyHaveThisDragonfly)
        (:then_1
          (if _have_it_already_
            (bind _returnvalue_2 (UserInterface|CreateWidget "/Game/SpyroContent/Global_Assets/Global_UserInterface/Widgets/YouAlreadyHaveThisX.YouAlreadyHaveThisX_C"))
            (Rendering|Components|TextRender|SetText (Variables|/Game/SpyroContent/Global_Assets/Global_UserInterface/Widgets/YouAlreadyHaveThisX.YouAlreadyHaveThisX_C|GetTextBlock_YouAlreadyHaveThisX _returnvalue_2) "You already have this dragonfly")
            (UserInterface|Viewport|AddtoViewport _returnvalue_2 0)
            (Default|DelayedSelf-Destruct _returnvalue_2 2.1)
            (else
              (if (Utilities|Enum|Equal(Enum) (Variables|Default|GetType%20Of%20Collectable) "NewEnumerator1")
                (bind _asspyro_player_controller (Utilities|Casting|CastToSpyro_PlayerController (Game|GetPlayerController 0)))
                (Default|ShowPrimaryCollectibleHUD _asspyro_player_controller 3.0))
              (bind _asspyro_persistant_data (Utilities|Casting|CastToSpyro_PersistantData (Game|GetGameInstance)))
              (Default|SaveACollectible _asspyro_persistant_data (Variables|Default|GetType%20Of%20Collectable) "" 2.1 (Variables|/Game/SpyroContent/Global_Assets/Global_Components/NPC_Award_Item.NPC_Award_Item_C|GetLevel%20Item%20Index (Variables|Default|GetNPC_Award_Item)) (Variables|Default|GetSkill%20Level%20Award))))
          (Effects|SpawnEmitteratLocation (Variables|Default|GetVFX) _returnvalue)
          (Audio|PlaySoundatLocation (Variables|Default|GetSFX) _returnvalue "0, 0, 0" 1.0 1.0 0.0 "/Game/SpyroContent/Global_Assets/Global_Audio/Attenuation/Spyro_Attenuation_MediumHigh.Spyro_Attenuation_MediumHigh" 0 0)
          (if (Variables|Default|GetI%20Am%20An%20NPC%20Award)
            (Input|EnableInput _player_who_was_awarded_me _spyrocontr_ref)
            (Variables|/Game/SpyroContent/Global_Assets/Global_Characters/Playable_Characters/BP_Base_Playable.BP_Base_Playable_C|SetDid%20we%20disable%20input? _player_who_was_awarded_me false)
            (Default|HideBlackBars _spyrocontr_ref)
            (Game|Player|SetViewTargetwithBlend _spyrocontr_ref _player_who_was_awarded_me 1.0 "VTBlend_Linear" 0.0 false)
            (bind _npc_who_awarded_me (Variables|/Game/SpyroContent/Global_Assets/Global_Components/NPC_Award_Item.NPC_Award_Item_C|GetNPC%20Who%20Awarded%20Me (Variables|Default|GetNPC_Award_Item))
              (:then
                (Variables|/Game/SpyroContent/Global_Assets/Global_Characters/NPCs/NPC_Base_BP.NPC_Base_BP_C|SetItem%20Award%20is%20Happening _npc_who_awarded_me false))
              (:else)))
          (Actor|DestroyActor))))))

(event Custom|NPC%20Award%20Process
  (Variables|Default|SetI%20Am%20An%20NPC%20Award true)
  (bind _player_who_was_awarded_me (Variables|/Game/SpyroContent/Global_Assets/Global_Components/NPC_Award_Item.NPC_Award_Item_C|GetPlayer%20Who%20Was%20Awarded%20Me (Variables|Default|GetNPC_Award_Item))
    (:then
      (Variables|Default|SetPlayer%20Who%20Was%20Awarded%20Me _player_who_was_awarded_me)
      (Transformation|SetActorRotation "0,-90.000000, 0")
      (Transformation|SetActorLocation (+ (Transformation|GetActorLocation) "0, 0,60.000000") false false)
      (CallFunction|CaptureSequence))
    (:else)))

(event EventBeginPlay
  (bind _skeletalmesh (Variables|Default|GetSkeletalMesh))
  (Variables|Default|SetSpawnLocation (Transformation|GetActorLocation))
  (Utilities|Time|SetTimerbyEvent (delegate Custom|UpdateErraticAngle) (Variables|Default|GetErraticChangeInterval) true)
  (bind _returnvalue (Rendering|Material|CreateDynamicMaterialInstance _skeletalmesh 0 (Rendering|Material|GetMaterial _skeletalmesh 0) "None" :!class /Script/Engine.PrimitiveComponent))
  (Rendering|Material|SetVectorParameterValue _returnvalue "ColorChange" (Variables|Default|GetDragonfly%20Color) :!class /Script/Engine.MaterialInstanceDynamic)
  (EventDispatchers|BindEventtoNPCAwardSpawned (Variables|Default|GetNPC_Award_Item) (delegate Custom|NPC%20Award%20Process)))

(event EventTick
  (params (DeltaSeconds :type Float%20%28single-precision%29))
  (bind _returnvalue (Game|GetPlayerCharacter 0))
  (bind _returnvalue_2 (Transformation|GetActorLocation))
  (bind _spawnlocation (Variables|Default|GetSpawnLocation))
  (bind _maxwanderradius (Variables|Default|GetMaxWanderRadius))
  (bind _returnvalue_3 (Transformation|GetActorLocation _returnvalue))
  (bind _z (Math|Vector|BreakVector _spawnlocation))
  (if (not (or (Variables|Default|GetI%20Am%20An%20NPC%20Award) (Variables|Default|GetI%20was%20captured)))
    (Variables|Default|SetCurrent%20Player%20Location%20%28Flattened%29 (Math|Vector|MakeVector (.x _returnvalue_3) (.y _returnvalue_3) _z))
    (Variables|Default|SetCurrent%20Dragonfly%20Location%20%28Flattened%29 (Math|Vector|MakeVector (.x _returnvalue_2) (.y _returnvalue_2) _z))
    (if (Variables|Default|GetisAlert)
      (if (> (Math|Vector|Distance(Vector) (Variables|Default|GetCurrent%20Dragonfly%20Location%20%28Flattened%29) (Variables|Default|GetCurrent%20Player%20Location%20%28Flattened%29)) (Variables|Default|GetUnalertRadius))
        (Variables|Default|SetisAlert false))
      (elif (< (Math|Vector|Distance(Vector) (Variables|Default|GetCurrent%20Dragonfly%20Location%20%28Flattened%29) (Variables|Default|GetCurrent%20Player%20Location%20%28Flattened%29)) (Variables|Default|GetAlertRadius))
        (Variables|Default|SetisAlert true)))
    (if (Variables|Default|GetisAlert)
      (Variables|Default|SetFinalFlightDirection (Math|Vector|Normalize (Math|Vector|Lerp(Vector) (Math|Vector|RotateVectorAroundAxis (Math|Vector|Normalize (- (Variables|Default|GetCurrent%20Dragonfly%20Location%20%28Flattened%29) (Variables|Default|GetCurrent%20Player%20Location%20%28Flattened%29))) (Variables|Default|GetCurrentErraticAngle) "0, 0,1.000000") (Math|Vector|Normalize (- (Variables|Default|GetSpawnLocation) (Variables|Default|GetCurrent%20Dragonfly%20Location%20%28Flattened%29))) (Math|Float|MapRangeClamped (Math|Vector|Distance(Vector) (Variables|Default|GetCurrent%20Dragonfly%20Location%20%28Flattened%29) (Variables|Default|GetSpawnLocation)) (* _maxwanderradius 0.6) _maxwanderradius 0.0 1.0))))
      (elif (< (Math|Vector|Distance(Vector) (Variables|Default|GetCurrent%20Dragonfly%20Location%20%28Flattened%29) (Variables|Default|GetSpawnLocation)) 2e+01)
        (Variables|Default|SetFinalFlightDirection "0, 0, 0")
        (else
          (Variables|Default|SetFinalFlightDirection (Math|Vector|Normalize (- (Variables|Default|GetSpawnLocation) (Variables|Default|GetCurrent%20Dragonfly%20Location%20%28Flattened%29)))))))
    (Transformation|SetActorLocation (Math|Vector|MakeVector (.X (Math|Vector|BreakVector (+ (Variables|Default|GetCurrent%20Dragonfly%20Location%20%28Flattened%29) (* (* (Variables|Default|GetFinalFlightDirection) (Variables|Default|GetFlySpeed)) (Utilities|Time|GetWorldDeltaSeconds))))) (.Y (Math|Vector|BreakVector (+ (Variables|Default|GetCurrent%20Dragonfly%20Location%20%28Flattened%29) (* (* (Variables|Default|GetFinalFlightDirection) (Variables|Default|GetFlySpeed)) (Utilities|Time|GetWorldDeltaSeconds))))) (.Z (Math|Vector|BreakVector (Variables|Default|GetSpawnLocation)))) true false)
    (if (not (Math|Vector|VectorIsNearlyZero (Variables|Default|GetFinalFlightDirection)))
      (Transformation|SetActorRotation (Math|Interpolation|RInterpTo (Transformation|GetActorRotation) (Math|Conversions|RotationFromXVector (Variables|Default|GetFinalFlightDirection)) (Utilities|Time|GetWorldDeltaSeconds) (Variables|Default|GetRotationSpeed))))))

(fn ConstructionScript)