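; BP_WipeSaveData is a utility actor that wipes collected-gem and level-item save data for the current save slot and level.
; One second after BeginPlay, it loads the current level's save named in the game instance and clears the gem collection matching the active slot (0–5).
; It saves that, then loads the Spyro_SaveData stored under its SlotName variable, clears all LevelItemInfo and saves again.
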(event EventBeginPlay
  (Utilities|FlowControl|Delay 1.0)
  (bind _asspyro_persistant_data (Utilities|Casting|CastToSpyro_PersistantData (Game|GetGameInstance)))
  (bind _returnvalue (SaveGame|LoadGamefromSlot (Variables|/Game/SpyroContent/Global_Assets/Global_SaveData/Spyro_PersistantData.Spyro_PersistantData_C|GetCurrent_Level_Name _asspyro_persistant_data)))
  (bind _asindividual_level_save_data (Utilities|Casting|CastToIndividual_Level_SaveData _returnvalue))
  (switch int (Variables|/Game/SpyroContent/Global_Assets/Global_SaveData/Spyro_PersistantData.Spyro_PersistantData_C|GetCurrent_SaveSlot _asspyro_persistant_data)
    (:0
      (Utilities|Array|Clear (Variables|/Game/SpyroContent/Global_Assets/Global_SaveData/Individual_Level_SaveData.Individual_Level_SaveData_C|Get0_Collected_Gems _asindividual_level_save_data)))
    (:1
      (Utilities|Array|Clear (Variables|/Game/SpyroContent/Global_Assets/Global_SaveData/Individual_Level_SaveData.Individual_Level_SaveData_C|Get1_Collected_Gems _asindividual_level_save_data)))
    (:2
      (Utilities|Array|Clear (Variables|/Game/SpyroContent/Global_Assets/Global_SaveData/Individual_Level_SaveData.Individual_Level_SaveData_C|Get2_Collected_Gems _asindividual_level_save_data)))
    (:3
      (Utilities|Array|Clear (Variables|/Game/SpyroContent/Global_Assets/Global_SaveData/Individual_Level_SaveData.Individual_Level_SaveData_C|Get3_Collected_Gems _asindividual_level_save_data)))
    (:4
      (Utilities|Array|Clear (Variables|/Game/SpyroContent/Global_Assets/Global_SaveData/Individual_Level_SaveData.Individual_Level_SaveData_C|Get4_Collected_Gems _asindividual_level_save_data)))
    (:5
      (Utilities|Array|Clear (Variables|/Game/SpyroContent/Global_Assets/Global_SaveData/Individual_Level_SaveData.Individual_Level_SaveData_C|Get5_Collected_Gems _asindividual_level_save_data))))
  (SaveGame|SaveGametoSlot _asindividual_level_save_data (Variables|/Game/SpyroContent/Global_Assets/Global_SaveData/Spyro_PersistantData.Spyro_PersistantData_C|GetCurrent_Level_Name _asspyro_persistant_data))
  (bind _returnvalue_2 (SaveGame|LoadGamefromSlot (Variables|Default|GetSlot%20Name)))
  (bind _asspyro_save_data (Utilities|Casting|CastToSpyro_SaveData _returnvalue_2))
  (Utilities|Array|Clear (Variables|/Game/SpyroContent/Global_Assets/Global_SaveData/Spyro_SaveData.Spyro_SaveData_C|GetLevel_Item_Info _asspyro_save_data))
  (SaveGame|SaveGametoSlot _asspyro_save_data (Variables|Default|GetSlot%20Name)))

(fn ConstructionScript)