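; BP_Whirlwind_Spawner is a trigger that turns on a whirlwind when the player enters its box.
; On BeginPlay it waits briefly, then deactivates the whirlwind, hides its particles and mutes its audio; the delay works around particles failing to reappear.
; When a BP_Base_Playable capsule overlaps the box, it activates the whirlwind, shows the particles and restores the volume, with no logic to switch it back off.
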(event OnComponentBeginOverlap(Box)
  (params (OverlappedComponent :type Primitive%20Component%20Object%20Reference) (OtherActor :type Actor%20Object%20Reference) (OtherComp :type Primitive%20Component%20Object%20Reference) (OtherBodyIndex :type Integer) (bFromSweep :type Boolean) (SweepResult :type Hit%20Result%20Structure%20%28by%20ref%29))
  (bind _whirlwind (Variables|Default|GetWhirlwind))
  (bind _asbp_base_playable (Utilities|Casting|CastToBP_Base_Playable OtherActor))
  (if (== (Variables|/Script/Engine.Character|GetCapsuleComponent _asbp_base_playable) OtherComp)
    (Variables|/Game/SpyroContent/Global_Assets/Global_Level_Items/Whirlwind/BP_Whirlwind.BP_Whirlwind_C|SetActive _whirlwind true)
    (Rendering|SetVisibility (Variables|/Game/SpyroContent/Global_Assets/Global_Level_Items/Whirlwind/BP_Whirlwind.BP_Whirlwind_C|GetWhirwind_Particles _whirlwind) true false)
    (Audio|Components|Audio|SetVolumeMultiplier (Variables|/Game/SpyroContent/Global_Assets/Global_Level_Items/Whirlwind/BP_Whirlwind.BP_Whirlwind_C|GetAudio _whirlwind) 1.0 :!class /Script/Engine.AudioComponent)))

(event EventBeginPlay
  (bind _whirlwind (Variables|Default|GetWhirlwind))
  ;[0 0 0 1 12] Sometimes the whirlwind particles wouldn't come back after they have been made visible again. A delay here seems to fix that
  (Utilities|FlowControl|Delay 0.2)
  (Variables|/Game/SpyroContent/Global_Assets/Global_Level_Items/Whirlwind/BP_Whirlwind.BP_Whirlwind_C|SetActive _whirlwind false)
  (Rendering|SetVisibility (Variables|/Game/SpyroContent/Global_Assets/Global_Level_Items/Whirlwind/BP_Whirlwind.BP_Whirlwind_C|GetWhirwind_Particles _whirlwind) false false)
  (Audio|Components|Audio|SetVolumeMultiplier (Variables|/Game/SpyroContent/Global_Assets/Global_Level_Items/Whirlwind/BP_Whirlwind.BP_Whirlwind_C|GetAudio _whirlwind) 0.0 :!class /Script/Engine.AudioComponent))

(fn ConstructionScript)