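; Trigger actor that opens a pair of banana plants when a playable character reaches it.
; On BeginPlay it closes both referenced banana plants.
; When the capsule of a BP_Base_Playable begins overlapping its box, it calls open on both plants.
; Nothing here closes them again after the overlap.
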(event OnComponentBeginOverlap(Box)
  (params (OverlappedComponent :type Primitive%20Component%20Object%20Reference) (OtherActor :type Actor%20Object%20Reference) (OtherComp :type Primitive%20Component%20Object%20Reference) (OtherBodyIndex :type Integer) (bFromSweep :type Boolean) (SweepResult :type Hit%20Result%20Structure%20%28by%20ref%29))
  (bind _asbp_base_playable (Utilities|Casting|CastToBP_Base_Playable OtherActor))
  (if (== (Variables|/Script/Engine.Character|GetCapsuleComponent _asbp_base_playable) OtherComp)
    (Default|OpenBananaPlant (Variables|Default|GetBanana%20Plant%201))))

(event EventBeginPlay
  (Default|CloseBananaPlant (Variables|Default|GetBanana%20Plant%201)))

(fn ConstructionScript)