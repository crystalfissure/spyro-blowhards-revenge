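; Utility actor that hides the level's portals at game start by moving them out of the way.
; On BeginPlay, if the HidePortals flag is set, it finds every BP_Portal actor and lowers it by a large fixed Z offset, keeping rotation and scale.
; The portals are only displaced, not destroyed or made invisible, and nothing in this Blueprint moves them back.
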(event EventBeginPlay
  (if (Variables|Default|GetHide%20Portals)
    (bind _outactors (Actor|GetAllActorsOfClass "/Game/SpyroContent/Global_Assets/Global_Level_Items/Portals/Actors/BP_Portal.BP_Portal_C"))
    (for _array_element _outactors
      (Transformation|SetActorTransform _array_element (Math|Transform|MakeTransform (Math|Vector|MakeVector (.X (Math|Vector|BreakVector (.Location (Math|Transform|BreakTransform (Transformation|GetActorTransform _array_element))))) (.Y (Math|Vector|BreakVector (.Location (Math|Transform|BreakTransform (Transformation|GetActorTransform _array_element))))) (- (.Z (Math|Vector|BreakVector (.Location (Math|Transform|BreakTransform (Transformation|GetActorTransform _array_element))))) 1.5e+04)) (.Rotation (Math|Transform|BreakTransform (Transformation|GetActorTransform _array_element))) (.Scale (Math|Transform|BreakTransform (Transformation|GetActorTransform _array_element))))))))

(event Collision|EventActorBeginOverlap
  (params (OtherActor :type Actor%20Object%20Reference)))

(event EventTick
  (params (DeltaSeconds :type Float%20%28single-precision%29)))

(fn ConstructionScript)