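; Utility actor that moves a skybox mesh to a configured height when play begins.
; After a one-second delay, it searches all BP_Skybox actors for the one nearest the world origin (not this actor), within the initial MinDistance.
; A timeline, with play rate set from LerpSpeed, then interpolates that skybox's static mesh relative Z from zero to SkyboxHeight.
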(event EventBeginPlay
  (Components|Timeline|SetPlayRate (Variables|Default|GetTimeline_0) (Variables|Default|GetLerp%20Speed))
  (Utilities|FlowControl|Delay 1.0)
  (bind _outactors (Actor|GetAllActorsOfClass "/Game/SpyroContent/Global_Assets/Global_Level_Items/Portals/Actors/BP_Skybox.BP_Skybox_C"))
  (for _array_element _outactors
    (if (< (Math|Vector|VectorLength (Transformation|GetActorLocation _array_element)) (Variables|Default|GetMinDistance))
      (Variables|Default|SetMinDistance (Math|Vector|VectorLength (Transformation|GetActorLocation _array_element)))
      (Variables|Default|SetClosest%20Skybox _array_element)))
  (Utilities|IsValid (Variables|Default|GetClosest%20Skybox)
    (:Is%20Valid
      (bind _newtrack_0 (Timeline|Timeline_0 Play)
        (:Update
          (Transformation|SetRelativeLocation (Variables|/Game/SpyroContent/Global_Assets/Global_Level_Items/Portals/Actors/BP_Skybox.BP_Skybox_C|GetStaticMesh (Variables|Default|GetClosest%20Skybox)) (Math|Vector|MakeVector 0.0 0.0 (Math|Float|Lerp 0.0 (Variables|Default|GetSkybox%20Height) _newtrack_0)) false false))))))

(fn ConstructionScript)