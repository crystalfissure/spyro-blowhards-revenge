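; BP_Yeetwind_Spawner is a trigger that activates a referenced Yeetwind when a player enters its box, rather than creating one at runtime.
; On BeginPlay, or when HideHurlwind is called, it sets the Yeetwind inactive and hides its particles.
; A box overlap by the capsule component of a BP_Base_Playable reactivates the Yeetwind and shows the particles.
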(event OnComponentBeginOverlap(Box)
  (params (OverlappedComponent :type Primitive%20Component%20Object%20Reference) (OtherActor :type Actor%20Object%20Reference) (OtherComp :type Primitive%20Component%20Object%20Reference) (OtherBodyIndex :type Integer) (bFromSweep :type Boolean) (SweepResult :type Hit%20Result%20Structure%20%28by%20ref%29))
  (bind _yeetwind (Variables|Default|GetYeetwind))
  (bind _asbp_base_playable (Utilities|Casting|CastToBP_Base_Playable OtherActor))
  (if (== (Variables|/Script/Engine.Character|GetCapsuleComponent _asbp_base_playable) OtherComp)
    (Variables|/Game/SpyroContent/Global_Assets/Global_Level_Items/Whirlwind/BP_Hurlwind.BP_Hurlwind_C|SetActive _yeetwind true)
    (Rendering|SetVisibility (Variables|/Game/SpyroContent/Global_Assets/Global_Level_Items/Whirlwind/BP_Hurlwind.BP_Hurlwind_C|GetHurlwind%20Particles _yeetwind) true false)))

(event Custom|Hide%20Hurlwind
  (bind _yeetwind (Variables|Default|GetYeetwind))
  (Variables|/Game/SpyroContent/Global_Assets/Global_Level_Items/Whirlwind/BP_Hurlwind.BP_Hurlwind_C|SetActive _yeetwind false)
  (Rendering|SetVisibility (Variables|/Game/SpyroContent/Global_Assets/Global_Level_Items/Whirlwind/BP_Hurlwind.BP_Hurlwind_C|GetHurlwind%20Particles _yeetwind) false false))

(event EventBeginPlay
  (bind _yeetwind (Variables|Default|GetYeetwind))
  (Variables|/Game/SpyroContent/Global_Assets/Global_Level_Items/Whirlwind/BP_Hurlwind.BP_Hurlwind_C|SetActive _yeetwind false)
  (Rendering|SetVisibility (Variables|/Game/SpyroContent/Global_Assets/Global_Level_Items/Whirlwind/BP_Hurlwind.BP_Hurlwind_C|GetHurlwind%20Particles _yeetwind) false false))

(fn ConstructionScript)