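; Utility actor that tallies the number and total value of gems available in the level, counting on BeginPlay.
; It sums placed Gem_Base_BP actors, then scans the drop lists of treasure containers and enemies.
; Dropped gem classes have no instance to read, so their values are hardcoded by matching class display names.
; After a short delay it prints both totals; CountGems resets and recounts.
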(event Custom|Count%20Gems
  (Variables|Default|SetTotalGemValue 0)
  (Variables|Default|SetGemCount 0)
  (bind _outactors (Actor|GetAllActorsOfClass "/Game/SpyroContent/Global_Assets/Global_Level_Items/Gems/Actors/Gem_Base_BP.Gem_Base_BP_C"))
  (for _array_element _outactors
    (Variables|Default|SetTotalGemValue (+ (Variables|/Game/SpyroContent/Global_Assets/Global_Level_Items/Gems/Actors/Gem_Base_BP.Gem_Base_BP_C|GetValue _array_element) (Variables|Default|GetTotalGemValue)))
    (Variables|Default|SetGemCount (+ 1 (Variables|Default|GetGemCount))))
  (bind _outactors_2 (Actor|GetAllActorsOfClass "/Game/SpyroContent/Global_Assets/Global_Level_Items/Treasure_Containers/Treasure_Container_Base_BP.Treasure_Container_Base_BP_C"))
  (for _array_element_2 _outactors_2
    (for _array_element_3 (Variables|/Game/SpyroContent/Global_Assets/Global_Components/Drops_Items.Drops_Items_C|GetItems_to_Drop (Variables|/Game/SpyroContent/Global_Assets/Global_Level_Items/Treasure_Containers/Treasure_Container_Base_BP.Treasure_Container_Base_BP_C|GetItem_Drop_Component _array_element_2))
      (if (Utilities|Enum|Equal(Enum) (Utilities|GetClassDisplayName _array_element_3) "Gem_Red_BP_C")
        (Variables|Default|SetCurrentGemValue 1)
        (Variables|Default|SetTotalGemValue (+ (Variables|Default|GetCurrentGemValue) (Variables|Default|GetTotalGemValue)) :!label _label)
        (Variables|Default|SetGemCount (+ 1 (Variables|Default|GetGemCount)))
        (elif (Utilities|Enum|Equal(Enum) (Utilities|GetClassDisplayName _array_element_3) "Gem_Green_BP_C")
          (Variables|Default|SetCurrentGemValue 2)
          (goto _label)
          (elif (Utilities|Enum|Equal(Enum) (Utilities|GetClassDisplayName _array_element_3) "Gem_Blueish_Purple_BP_C")
            (Variables|Default|SetCurrentGemValue 5)
            (goto _label)
            (elif (Utilities|Enum|Equal(Enum) (Utilities|GetClassDisplayName _array_element_3) "Gem_Yellow_BP_C")
              (Variables|Default|SetCurrentGemValue 10)
              (goto _label)
              (elif (Utilities|Enum|Equal(Enum) (Utilities|GetClassDisplayName _array_element_3) "Gem_Magenta_BP_C")
                (Variables|Default|SetCurrentGemValue 25)
                (goto _label)
                (elif (Utilities|Enum|Equal(Enum) (Utilities|GetClassDisplayName _array_element_3) "Gem_Orange_BP_C")
                  (Variables|Default|SetCurrentGemValue 50)
                  (goto _label)
                  (elif (Utilities|Enum|Equal(Enum) (Utilities|GetClassDisplayName _array_element_3) "Gem_Cyan_BP_C")
                    (Variables|Default|SetCurrentGemValue 100)
                    (goto _label))))))))))
  (bind _outactors_3 (Actor|GetAllActorsOfClass "/Game/SpyroContent/Global_Assets/Global_Characters/AI_Characters/Actors/Enemies/Base_Enemy_BP.Base_Enemy_BP_C"))
  (for _array_element_4 _outactors_3
    (for _array_element_5 (Variables|/Game/SpyroContent/Global_Assets/Global_Components/Drops_Items.Drops_Items_C|GetItems_to_Drop (Variables|/Game/SpyroContent/Global_Assets/Global_Characters/AI_Characters/Actors/Base_AICharacter_BP.Base_AICharacter_BP_C|GetDrops_Items _array_element_4))
      (if (Utilities|Enum|Equal(Enum) (Utilities|GetClassDisplayName _array_element_5) "Gem_Red_BP_C")
        (Variables|Default|SetCurrentGemValue 1)
        (Variables|Default|SetTotalGemValue (+ (Variables|Default|GetCurrentGemValue) (Variables|Default|GetTotalGemValue)) :!label _label_2)
        (Variables|Default|SetGemCount (+ 1 (Variables|Default|GetGemCount)))
        (elif (Utilities|Enum|Equal(Enum) (Utilities|GetClassDisplayName _array_element_5) "Gem_Green_BP_C")
          (Variables|Default|SetCurrentGemValue 2)
          (goto _label_2)
          (elif (Utilities|Enum|Equal(Enum) (Utilities|GetClassDisplayName _array_element_5) "Gem_Blueish_Purple_BP_C")
            (Variables|Default|SetCurrentGemValue 5)
            (goto _label_2)
            (elif (Utilities|Enum|Equal(Enum) (Utilities|GetClassDisplayName _array_element_5) "Gem_Yellow_BP_C")
              (Variables|Default|SetCurrentGemValue 10)
              (goto _label_2)
              (elif (Utilities|Enum|Equal(Enum) (Utilities|GetClassDisplayName _array_element_5) "Gem_Magenta_BP_C")
                (Variables|Default|SetCurrentGemValue 25)
                (goto _label_2)
                (elif (Utilities|Enum|Equal(Enum) (Utilities|GetClassDisplayName _array_element_5) "Gem_Orange_BP_C")
                  (Variables|Default|SetCurrentGemValue 50)
                  (goto _label_2)
                  (elif (Utilities|Enum|Equal(Enum) (Utilities|GetClassDisplayName _array_element_5) "Gem_Cyan_BP_C")
                    (Variables|Default|SetCurrentGemValue 100)
                    (goto _label_2))))))))))
  (Utilities|FlowControl|Delay 0.5)
  (Development|PrintString (Utilities|String|BuildString(Integer) "" "TOTAL GEM VALUE: " (Variables|Default|GetTotalGemValue)))
  (Development|PrintString (Utilities|String|BuildString(Integer) "" "GEM COUNT: " (Variables|Default|GetGemCount))))

(event EventBeginPlay
  (bind _outactors (Actor|GetAllActorsOfClass "/Game/SpyroContent/Global_Assets/Global_Level_Items/Gems/Actors/Gem_Base_BP.Gem_Base_BP_C"))
  (for _array_element _outactors
    (Variables|Default|SetTotalGemValue (+ (Variables|/Game/SpyroContent/Global_Assets/Global_Level_Items/Gems/Actors/Gem_Base_BP.Gem_Base_BP_C|GetValue _array_element) (Variables|Default|GetTotalGemValue)))
    (Variables|Default|SetGemCount (+ 1 (Variables|Default|GetGemCount))))
  (bind _outactors_2 (Actor|GetAllActorsOfClass "/Game/SpyroContent/Global_Assets/Global_Level_Items/Treasure_Containers/Treasure_Container_Base_BP.Treasure_Container_Base_BP_C"))
  (for _array_element_2 _outactors_2
    (for _array_element_3 (Variables|/Game/SpyroContent/Global_Assets/Global_Components/Drops_Items.Drops_Items_C|GetItems_to_Drop (Variables|/Game/SpyroContent/Global_Assets/Global_Level_Items/Treasure_Containers/Treasure_Container_Base_BP.Treasure_Container_Base_BP_C|GetItem_Drop_Component _array_element_2))
      (if (Utilities|Enum|Equal(Enum) (Utilities|GetClassDisplayName _array_element_3) "Gem_Red_BP_C")
        (Variables|Default|SetCurrentGemValue 1)
        (Variables|Default|SetTotalGemValue (+ (Variables|Default|GetCurrentGemValue) (Variables|Default|GetTotalGemValue)) :!label _label)
        (Variables|Default|SetGemCount (+ 1 (Variables|Default|GetGemCount)))
        (elif (Utilities|Enum|Equal(Enum) (Utilities|GetClassDisplayName _array_element_3) "Gem_Green_BP_C")
          (Variables|Default|SetCurrentGemValue 2)
          (goto _label)
          (elif (Utilities|Enum|Equal(Enum) (Utilities|GetClassDisplayName _array_element_3) "Gem_Blueish_Purple_BP_C")
            (Variables|Default|SetCurrentGemValue 5)
            (goto _label)
            (elif (Utilities|Enum|Equal(Enum) (Utilities|GetClassDisplayName _array_element_3) "Gem_Yellow_BP_C")
              (Variables|Default|SetCurrentGemValue 10)
              (goto _label)
              (elif (Utilities|Enum|Equal(Enum) (Utilities|GetClassDisplayName _array_element_3) "Gem_Magenta_BP_C")
                (Variables|Default|SetCurrentGemValue 25)
                (goto _label)
                (elif (Utilities|Enum|Equal(Enum) (Utilities|GetClassDisplayName _array_element_3) "Gem_Orange_BP_C")
                  (Variables|Default|SetCurrentGemValue 50)
                  (goto _label)
                  (elif (Utilities|Enum|Equal(Enum) (Utilities|GetClassDisplayName _array_element_3) "Gem_Cyan_BP_C")
                    (Variables|Default|SetCurrentGemValue 100)
                    (goto _label))))))))))
  (bind _outactors_3 (Actor|GetAllActorsOfClass "/Game/SpyroContent/Global_Assets/Global_Characters/AI_Characters/Actors/Enemies/Base_Enemy_BP.Base_Enemy_BP_C"))
  (for _array_element_4 _outactors_3
    (for _array_element_5 (Variables|/Game/SpyroContent/Global_Assets/Global_Components/Drops_Items.Drops_Items_C|GetItems_to_Drop (Variables|/Game/SpyroContent/Global_Assets/Global_Characters/AI_Characters/Actors/Base_AICharacter_BP.Base_AICharacter_BP_C|GetDrops_Items _array_element_4))
      (if (Utilities|Enum|Equal(Enum) (Utilities|GetClassDisplayName _array_element_5) "Gem_Red_BP_C")
        (Variables|Default|SetCurrentGemValue 1)
        (Variables|Default|SetTotalGemValue (+ (Variables|Default|GetCurrentGemValue) (Variables|Default|GetTotalGemValue)) :!label _label_2)
        (Variables|Default|SetGemCount (+ 1 (Variables|Default|GetGemCount)))
        (elif (Utilities|Enum|Equal(Enum) (Utilities|GetClassDisplayName _array_element_5) "Gem_Green_BP_C")
          (Variables|Default|SetCurrentGemValue 2)
          (goto _label_2)
          (elif (Utilities|Enum|Equal(Enum) (Utilities|GetClassDisplayName _array_element_5) "Gem_Blueish_Purple_BP_C")
            (Variables|Default|SetCurrentGemValue 5)
            (goto _label_2)
            (elif (Utilities|Enum|Equal(Enum) (Utilities|GetClassDisplayName _array_element_5) "Gem_Yellow_BP_C")
              (Variables|Default|SetCurrentGemValue 10)
              (goto _label_2)
              (elif (Utilities|Enum|Equal(Enum) (Utilities|GetClassDisplayName _array_element_5) "Gem_Magenta_BP_C")
                (Variables|Default|SetCurrentGemValue 25)
                (goto _label_2)
                (elif (Utilities|Enum|Equal(Enum) (Utilities|GetClassDisplayName _array_element_5) "Gem_Orange_BP_C")
                  (Variables|Default|SetCurrentGemValue 50)
                  (goto _label_2)
                  (elif (Utilities|Enum|Equal(Enum) (Utilities|GetClassDisplayName _array_element_5) "Gem_Cyan_BP_C")
                    (Variables|Default|SetCurrentGemValue 100)
                    (goto _label_2))))))))))
  (Utilities|FlowControl|Delay 0.5)
  (Development|PrintString (Utilities|String|BuildString(Integer) "" "TOTAL GEM VALUE: " (Variables|Default|GetTotalGemValue)))
  (Development|PrintString (Utilities|String|BuildString(Integer) "" "GEM COUNT: " (Variables|Default|GetGemCount))))

(event EventTick
  (params (DeltaSeconds :type Float%20%28single-precision%29)))

(fn ConstructionScript)