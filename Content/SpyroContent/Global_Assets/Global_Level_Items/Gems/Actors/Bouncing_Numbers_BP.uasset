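; Bouncing number pickup effect actor for the gem items, a physical number that bounces around briefly before popping.
; Tick spins NumberMesh around yaw while hits on CollissionMesh push it away along the surface normal with a velocity-change impulse.
; BeginPlay links a child Dropshadow_BP to NumberMesh, then after three seconds spawns a gold letter pop particle at the collision mesh and destroys the actor.
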(event OnComponentHit(CollissionMesh)
  (params (HitComponent :type Primitive%20Component%20Object%20Reference) (OtherActor :type Actor%20Object%20Reference) (OtherComp :type Primitive%20Component%20Object%20Reference) (NormalImpulse :type Vector :default "0, 0, 0") (Hit :type Hit%20Result%20Structure%20%28by%20ref%29))
  (Physics|AddImpulse (Variables|Default|GetCollission%20Mesh) (* (.normal Hit) 4e+02) "None" true))

(event EventBeginPlay
  (bind _asdropshadow_bp (Utilities|Casting|CastToDropshadow_BP (Variables|/Script/Engine.ChildActorComponent|GetChildActor (Variables|Default|GetDropshadow)))
    (:then
      (Variables|/Game/SpyroContent/Global_Assets/Global_Level_Items/Dropshadow/Dropshadow_BP.Dropshadow_BP_C|SetOwning%20Component _asdropshadow_bp (Variables|Default|GetNumber%20Mesh)))
    (:CastFailed
      _))
  (Utilities|FlowControl|Delay 3.0)
  (Effects|SpawnEmitteratLocation "/Game/SpyroContent/Global_Assets/Global_Level_Items/Gems/Particles/gold_letter_pop_particle.gold_letter_pop_particle" (Transformation|GetWorldLocation (Variables|Default|GetCollission%20Mesh)))
  (Actor|DestroyActor))

(event EventTick
  (params (DeltaSeconds :type Float%20%28single-precision%29))
  (Transformation|AddLocalRotation (Variables|Default|GetNumber%20Mesh) (Math|Rotator|MakeRotator 0.0 0.0 (* DeltaSeconds -4e+01)) false false))

(fn ConstructionScript)