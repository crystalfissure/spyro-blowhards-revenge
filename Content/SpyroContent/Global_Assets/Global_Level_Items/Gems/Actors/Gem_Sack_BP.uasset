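; Gem sack pickup tied to the player who spawned it, awarding all the gems it holds on overlap.
; Collection queues gems as pending on the controller, updates temporary level counts and HUD, then plays effects and destroys itself.
; Once bound, the owner's death hides the sack and blocks pickup; the pre-respawn event resets its gems and destroys it.
; BeginPlay traces down to place a drop shadow; level transitions destroy it.
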(event OnComponentBeginOverlap(Hitbox)
  (params (OverlappedComponent :type Primitive%20Component%20Object%20Reference) (OtherActor :type Actor%20Object%20Reference) (OtherComp :type Primitive%20Component%20Object%20Reference) (OtherBodyIndex :type Integer) (bFromSweep :type Boolean) (SweepResult :type Hit%20Result%20Structure%20%28by%20ref%29))
  (bind _returnvalue (Transformation|GetActorLocation))
  (bind _asbp_base_playable (Utilities|Casting|CastToBP_Base_Playable OtherActor))
  (if (Math|Boolean|ANDBoolean (== (Variables|/Script/Engine.Character|GetCapsuleComponent _asbp_base_playable) OtherComp) (not (Variables|/Game/SpyroContent/Global_Assets/Global_Characters/Playable_Characters/BP_Base_Playable.BP_Base_Playable_C|GetRespawning _asbp_base_playable)) (not (Utilities|Enum|Equal(Enum) (Variables|/Game/SpyroContent/Global_Assets/Global_Characters/Playable_Characters/BP_Base_Playable.BP_Base_Playable_C|GetPlayer_State _asbp_base_playable) "NewEnumerator11")) (not (Variables|/Game/SpyroContent/Global_Assets/Global_SaveData/Spyro_PersistantData.Spyro_PersistantData_C|GetPortal_Transition (Variables|/Game/SpyroContent/Global_Assets/Global_Characters/Playable_Characters/BP_Base_Playable.BP_Base_Playable_C|GetPersData_Ref _asbp_base_playable))) (not (Variables|Default|GetPoofed)))
    (Utilities|FlowControl|DoOnce false
      (:Completed
        (bind _asspyro_persistant_data (Utilities|Casting|CastToSpyro_PersistantData (Game|GetGameInstance)))
        (for _array_element (Variables|Default|GetGems_in_Sack)
          (Utilities|Array|AddUnique (Variables|/Game/SpyroContent/Global_Assets/Global_Characters/Playable_Characters/Spyro_PlayerController.Spyro_PlayerController_C|GetGems_Pending_Collection (Variables|/Game/SpyroContent/Global_Assets/Global_Characters/Playable_Characters/BP_Base_Playable.BP_Base_Playable_C|GetSpyroContr_Ref _asbp_base_playable)) _array_element)
          (bind _foundwidgets (Widget|GetAllWidgetsOfClass "/Game/SpyroContent/Global_Assets/Global_UserInterface/Widgets/HUD.HUD_C" true))
          (Utilities|Array|SetArrayElem (.individuallevelgemcount (Utilities|Array|Get(acopy) (Variables|/Game/SpyroContent/Global_Assets/Global_SaveData/Spyro_PersistantData.Spyro_PersistantData_C|GetTEMPORARY_Level_GemCounts _asspyro_persistant_data) (Variables|/Game/SpyroContent/Global_Assets/Global_SaveData/Spyro_PersistantData.Spyro_PersistantData_C|GetCurrent_Homeworld_Index _asspyro_persistant_data))) (Variables|/Game/SpyroContent/Global_Assets/Global_SaveData/Spyro_PersistantData.Spyro_PersistantData_C|GetCurrent_Level_Index _asspyro_persistant_data) (+ (Utilities|Array|Get(acopy) (.individuallevelgemcount (Utilities|Array|Get(acopy) (Variables|/Game/SpyroContent/Global_Assets/Global_SaveData/Spyro_PersistantData.Spyro_PersistantData_C|GetTEMPORARY_Level_GemCounts _asspyro_persistant_data) (Variables|/Game/SpyroContent/Global_Assets/Global_SaveData/Spyro_PersistantData.Spyro_PersistantData_C|GetCurrent_Homeworld_Index _asspyro_persistant_data))) (Variables|/Game/SpyroContent/Global_Assets/Global_SaveData/Spyro_PersistantData.Spyro_PersistantData_C|GetCurrent_Level_Index _asspyro_persistant_data)) (.GemValue (Utilities|Struct|BreakGem_Info _array_element))) true)
          (Variables|/Game/SpyroContent/Global_Assets/Global_UserInterface/Widgets/HUD.HUD_C|SetActual_HUD_Gems (Utilities|Array|Get(acopy) _foundwidgets) (+ (Variables|/Game/SpyroContent/Global_Assets/Global_UserInterface/Widgets/HUD.HUD_C|GetActual_HUD_Gems (Utilities|Array|Get(acopy) _foundwidgets)) (.GemValue (Utilities|Struct|BreakGem_Info _array_element))))
          (bind _asspyro_persistant_data_2 (Utilities|Casting|CastToSpyro_PersistantData (Game|GetGameInstance)))
          (Variables|/Game/SpyroContent/Global_Assets/Global_SaveData/Spyro_PersistantData.Spyro_PersistantData_C|SetGems_Collected_in_this_Level _asspyro_persistant_data_2 (+ (Variables|/Game/SpyroContent/Global_Assets/Global_SaveData/Spyro_PersistantData.Spyro_PersistantData_C|GetGems_Collected_in_this_Level _asspyro_persistant_data_2) (.GemValue (Utilities|Struct|BreakGem_Info _array_element))))
          (CallFunction|Increase/DecreaseGemColorCountby1 (.GemValue (Utilities|Struct|BreakGem_Info _array_element)) false self))
        (Audio|PlaySoundatLocation "/Game/SpyroContent/Global_Assets/Global_Level_Items/Gems/Audio/gem_collection.gem_collection" _returnvalue "0, 0, 0" 1.0 1.0 0.0 0 0 0)
        (bind _returnvalue_2 (Effects|SpawnEmitteratLocation "/Game/SpyroContent/Global_Assets/Global_Level_Items/Gems/Particles/Gem_Star_Burst.Gem_Star_Burst" _returnvalue))
        (bind _returnvalue_3 (Rendering|Material|CreateDynamicMaterialInstance _returnvalue_2 0 "/Game/SpyroContent/Global_Assets/Global_Level_Items/Gems/Materials/Material_Instances/Gem_Sparkle_Mat.Gem_Sparkle_Mat" "None" :!class /Script/Engine.PrimitiveComponent))
        (Rendering|Material|SetVectorParameterValue _returnvalue_3 "Color Multiplier" "(R=0.000000,G=0.658824,B=0.000000,A=1.000000)" :!class /Script/Engine.MaterialInstanceDynamic)
        (Default|ShowGemHUD (Variables|/Game/SpyroContent/Global_Assets/Global_Characters/Playable_Characters/BP_Base_Playable.BP_Base_Playable_C|GetSpyroContr_Ref _asbp_base_playable))
        (Actor|DestroyActor)))))

(event Custom|Self%20Destruct
  (Actor|DestroyActor))

(event Custom|Bind%20to%20Player
  (bind _player_who_spawned_me (Variables|Default|GetPlayer_Who_Spawned_Me)
    (:then
      (EventDispatchers|BindEventtoPlayerDied _player_who_spawned_me (delegate Custom|Poof%20the%20Bag))
      (EventDispatchers|BindEventtoAbouttoRespawn _player_who_spawned_me (delegate Custom|Drop%20My%20Gemss)))
    (:else)))

(event Custom|Poof%20the%20Bag
  (Utilities|FlowControl|DoOnce false
    (:Completed
      (Effects|SpawnEmitteratLocation "/Game/SpyroContent/Global_Assets/Global_Particles/dust_ring.dust_ring" (Transformation|GetActorLocation))
      (Rendering|SetVisibility (Variables|Default|GetStaticMesh) false false)
      (Variables|Default|SetPoofed true))))

(event Custom|Drop%20My%20Gemss
  (Utilities|FlowControl|DoOnce false
    (:Completed
      (for _array_element (Variables|Default|GetGems_in_Sack)
        (Utilities|IsValid (.gemobjectref _array_element)
          (:Is%20Valid
            (Default|ResetGem (.gemobjectref _array_element)))))
      (Actor|DestroyActor))))

(event EventBeginPlay
  (bind _returnvalue (Transformation|GetActorLocation))
  (bind (_x _y _z) (Math|Vector|BreakVector _returnvalue))
  (bind _outhit (Collision|LineTraceForObjects _returnvalue (Math|Vector|MakeVector _x _y (- _z 1e+03)) (Utilities|Array|MakeArray "ObjectTypeQuery1") false 0 "None"))
  (if (.bblockinghit _outhit)
    (Transformation|SetWorldLocation (Variables|Default|GetDrop_Shadow) (Math|Vector|MakeVector (.X (Math|Vector|BreakVector (.location _outhit))) (.Y (Math|Vector|BreakVector (.location _outhit))) (+ (.Z (Math|Vector|BreakVector (.location _outhit))) 5.0)) false false))
  (bind _asspyro_persistant_data (Utilities|Casting|CastToSpyro_PersistantData (Game|GetGameInstance)))
  (EventDispatchers|BindEventtoBeginLevelTransition _asspyro_persistant_data (delegate Custom|Self%20Destruct)))

(fn ConstructionScript)