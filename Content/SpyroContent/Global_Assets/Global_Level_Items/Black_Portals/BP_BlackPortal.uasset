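; Black portal that teleports the player to its linked SisterPortal behind a fade to black.
; Overlap disables input, pauses music and passes on the sister's sublevel and water state; after the fade it moves the player, updates respawn data and switches music.
; BeginPlay registers the portal in persistent data and stamps its sublevel index on nearby gems, players and drop items.
; A tiny control-yaw offset works around a walk-in-place bug.
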(event OnComponentBeginOverlap(Box)
  (params (OverlappedComponent :type Primitive%20Component%20Object%20Reference) (OtherActor :type Actor%20Object%20Reference) (OtherComp :type Primitive%20Component%20Object%20Reference) (OtherBodyIndex :type Integer) (bFromSweep :type Boolean) (SweepResult :type Hit%20Result%20Structure%20%28by%20ref%29))
  (CallFunction|OnBlackPortalOverlap OtherActor OtherComp))

(event OnComponentBeginOverlap(Music_HitBbox)
  (params (OverlappedComponent :type Primitive%20Component%20Object%20Reference) (OtherActor :type Actor%20Object%20Reference) (OtherComp :type Primitive%20Component%20Object%20Reference) (OtherBodyIndex :type Integer) (bFromSweep :type Boolean) (SweepResult :type Hit%20Result%20Structure%20%28by%20ref%29))
  (bind _asbp_base_playable (Utilities|Casting|CastToBP_Base_Playable OtherActor))
  (if (and (== (Variables|/Script/Engine.Character|GetCapsuleComponent _asbp_base_playable) OtherComp) (not (Variables|/Game/SpyroContent/Global_Assets/Global_Characters/Playable_Characters/BP_Base_Playable.BP_Base_Playable_C|GetIn_BlackPortal_Transition _asbp_base_playable)))
    (CallFunction|Pause/UnpauseMusic self true false)))

(event OnComponentEndOverlap(Music_HitBbox)
  (params (OverlappedComponent :type Primitive%20Component%20Object%20Reference) (OtherActor :type Actor%20Object%20Reference) (OtherComp :type Primitive%20Component%20Object%20Reference) (OtherBodyIndex :type Integer))
  (bind _asbp_base_playable (Utilities|Casting|CastToBP_Base_Playable OtherActor))
  (if (Math|Boolean|ANDBoolean (== (Variables|/Script/Engine.Character|GetCapsuleComponent _asbp_base_playable) OtherComp) (not (Variables|/Game/SpyroContent/Global_Assets/Global_Characters/Playable_Characters/BP_Base_Playable.BP_Base_Playable_C|GetIn_BlackPortal_Transition _asbp_base_playable)) (not (Variables|/Game/SpyroContent/Global_Assets/Global_SaveData/Spyro_PersistantData.Spyro_PersistantData_C|GetPortal_Transition (Variables|/Game/SpyroContent/Global_Assets/Global_Characters/Playable_Characters/BP_Base_Playable.BP_Base_Playable_C|GetPersData_Ref _asbp_base_playable))) (not (Variables|/Game/SpyroContent/Global_Assets/Global_Characters/Playable_Characters/BP_Base_Playable.BP_Base_Playable_C|GetDid%20we%20disable%20input? _asbp_base_playable)))
    (CallFunction|Pause/UnpauseMusic self false false)))

(event Custom|Fade%20From%20Black
  (bind _newtrack_0 (Timeline|Timeline_1 PlayFromStart)
    (:Update
      (Rendering|Material|SetScalarParameterValue "/Game/SpyroContent/Global_Assets/Global_Materials/View_Option_Scalars.View_Option_Scalars" "Fade_to_Black" (Math|Float|Lerp 1.0 0.0 _newtrack_0) :!class /Script/Engine.KismetMaterialLibrary))))

(event Custom|Fade%20to%20Black
  (bind _newtrack_0 (Timeline|Timeline_0 PlayFromStart)
    (:Update
      (Rendering|Material|SetScalarParameterValue "/Game/SpyroContent/Global_Assets/Global_Materials/View_Option_Scalars.View_Option_Scalars" "Fade_to_Black" (Math|Float|Lerp 0.0 1.0 _newtrack_0) :!class /Script/Engine.KismetMaterialLibrary))
    (:Finished
      (Utilities|FlowControl|Delay 0.5)
      (bind _sister_portal (Variables|Default|GetSister_Portal)
        (:then
          (CallFunction|ChangeMusic self (Variables|BP_BlackPortal_C|GetExit%20Music _sister_portal))
          (CallFunction|RestartMusic self)
          (Transformation|SetActorLocationAndRotation (Variables|Default|GetPlayer_In_Portal) (Math|Vector|MakeVector (.x (+ (Transformation|GetActorLocation _sister_portal) (* (Transformation|GetActorForwardVector _sister_portal) -4e+02))) (.y (+ (Transformation|GetActorLocation _sister_portal) (* (Transformation|GetActorForwardVector _sister_portal) -4e+02))) (- (.z (+ (Transformation|GetActorLocation _sister_portal) (* (Transformation|GetActorForwardVector _sister_portal) -4e+02))) (Variables|BP_BlackPortal_C|Getplayer%20height%20spawn%20offset _sister_portal))) (Math|Rotator|MakeRotator 0.0 0.0 (+ (.yaw (Transformation|GetActorRotation _sister_portal)) 1.8e+02)))
          (Variables|/Game/SpyroContent/Global_Assets/Global_Characters/Playable_Characters/BP_Base_Playable.BP_Base_Playable_C|SetPlayer_Respawn_Data (Variables|Default|GetPlayer_In_Portal) (Utilities|Struct|MakePlayer_Respawn_Data (Math|Transform|MakeTransform (Math|Vector|MakeVector (.x (+ (Transformation|GetActorLocation _sister_portal) (* (Transformation|GetActorForwardVector _sister_portal) -4e+02))) (.y (+ (Transformation|GetActorLocation _sister_portal) (* (Transformation|GetActorForwardVector _sister_portal) -4e+02))) (- (.z (+ (Transformation|GetActorLocation _sister_portal) (* (Transformation|GetActorForwardVector _sister_portal) -4e+02))) (Variables|BP_BlackPortal_C|Getplayer%20height%20spawn%20offset _sister_portal))) (Math|Rotator|MakeRotator 0.0 0.0 (+ (.yaw (Transformation|GetActorRotation _sister_portal)) 1.8e+02)) "1,1,1") (Utilities|Enum|Equal(Enum) (Variables|/Game/SpyroContent/Global_Assets/Global_Characters/Playable_Characters/BP_Base_Playable.BP_Base_Playable_C|GetEnvironmental_State (Variables|Default|GetPlayer_In_Portal)) "NewEnumerator1")))
          (Pawn|SetControlRotation (Pawn|GetController (Variables|Default|GetPlayer_In_Portal)) (Math|Rotator|MakeRotator (.Roll (Math|Rotator|BreakRotator (Math|Rotator|MakeRotator 0.0 0.0 (+ (.yaw (Transformation|GetActorRotation _sister_portal)) 1.8e+02)))) (.Pitch (Math|Rotator|BreakRotator (Math|Rotator|MakeRotator 0.0 0.0 (+ (.yaw (Transformation|GetActorRotation _sister_portal)) 1.8e+02)))) (+ (.Yaw (Math|Rotator|BreakRotator (Math|Rotator|MakeRotator 0.0 0.0 (+ (.yaw (Transformation|GetActorRotation _sister_portal)) 1.8e+02)))) 0.001)))
          (CallFunction|FadefromBlack)
          (Variables|/Game/SpyroContent/Global_Assets/Global_Characters/Playable_Characters/BP_Base_Playable.BP_Base_Playable_C|SetBlackPortal_Skid (Variables|Default|GetPlayer_In_Portal) true)
          (bind _assparx_bp (Utilities|Casting|CastToSparx_BP (Variables|/Script/Engine.ChildActorComponent|GetChildActor (Variables|/Game/SpyroContent/Global_Assets/Global_Characters/Playable_Characters/BP_Base_Playable.BP_Base_Playable_C|GetSparx (Variables|Default|GetPlayer_In_Portal))))
            (:then
              (Default|FlyinfromOffCamera _assparx_bp))
            (:CastFailed
              _))
          (Utilities|FlowControl|Delay 0.5)
          (Variables|/Game/SpyroContent/Global_Assets/Global_Characters/Playable_Characters/BP_Base_Playable.BP_Base_Playable_C|SetBlackPortal_Skid (Variables|Default|GetPlayer_In_Portal) false)
          (bind _asplayer_controller (Utilities|Casting|CastToPlayerController (Pawn|GetController (Variables|Default|GetPlayer_In_Portal))))
          (Variables|/Game/SpyroContent/Global_Assets/Global_Characters/Playable_Characters/BP_Base_Playable.BP_Base_Playable_C|GetTalking_NPC (Variables|Default|GetPlayer_In_Portal)
            (:then
              _)
            (:else
              (Input|EnableInput (Variables|Default|GetPlayer_In_Portal) _asplayer_controller)
              (Variables|/Game/SpyroContent/Global_Assets/Global_Characters/Playable_Characters/BP_Base_Playable.BP_Base_Playable_C|SetDid%20we%20disable%20input? (Variables|Default|GetPlayer_In_Portal) false)))
          (Variables|/Game/SpyroContent/Global_Assets/Global_Characters/Playable_Characters/BP_Base_Playable.BP_Base_Playable_C|SetIn_BlackPortal_Transition (Variables|Default|GetPlayer_In_Portal) false)
          (Variables|Default|SetPlayer_In_Portal 0)
          (Collision|SetCollisionEnabled (Variables|Default|GetStaticMesh) "NoCollision"))
        (:else)))))

(event EventBeginPlay
  (bind _gem_detection_sphere (Variables|Default|GetGem_Detection_Sphere))
  (bind _returnvalue (Transformation|GetWorldLocation _gem_detection_sphere))
  (Class|ActorComponent|SetTickablewhenPaused (Variables|Default|GetTimeline_0) true)
  (bind _outhits (Collision|MultiSphereTraceForObjects _returnvalue _returnvalue (Variables|/Script/Engine.SphereComponent|GetSphereRadius _gem_detection_sphere) (Utilities|Array|MakeArray "ObjectTypeQuery1" "ObjectTypeQuery3" "ObjectTypeQuery2" "ObjectTypeQuery4") false 0 "None"))
  (for _array_element _outhits
    (Utilities|IsValid (.hitactor _array_element)
      (:Is%20Valid
        (bind _asgem_base_bp (Utilities|Casting|CastToGem_Base_BP (.hitactor _array_element))
          (:then
            (Variables|/Game/SpyroContent/Global_Assets/Global_Level_Items/Gems/Actors/Gem_Base_BP.Gem_Base_BP_C|SetMy%20Sublevel%20Index _asgem_base_bp (Variables|Default|GetMy%20Sublevel%20Index)))
          (:CastFailed
            (bind _asbp_base_playable (Utilities|Casting|CastToBP_Base_Playable (.hitactor _array_element))
              (:then
                (Variables|/Game/SpyroContent/Global_Assets/Global_Characters/Playable_Characters/BP_Base_Playable.BP_Base_Playable_C|SetMy%20Sublevel%20Index _asbp_base_playable (Variables|Default|GetMy%20Sublevel%20Index)))
              (:CastFailed
                (Utilities|IsValid (Actor|GetComponentbyClass (.hitactor _array_element) "/Game/SpyroContent/Global_Assets/Global_Components/Drops_Items.Drops_Items_C")
                  (:Is%20Valid
                    (Variables|/Game/SpyroContent/Global_Assets/Global_Components/Drops_Items.Drops_Items_C|SetMy%20Sublevel%20Index (Actor|GetComponentbyClass (.hitactor _array_element) "/Game/SpyroContent/Global_Assets/Global_Components/Drops_Items.Drops_Items_C") (Variables|Default|GetMy%20Sublevel%20Index)))))))))))
  (bind _asspyro_persistant_data (Utilities|Casting|CastToSpyro_PersistantData (Game|GetGameInstance)))
  (Utilities|Array|AddUnique (Variables|/Game/SpyroContent/Global_Assets/Global_SaveData/Spyro_PersistantData.Spyro_PersistantData_C|GetAll_BlackPortals _asspyro_persistant_data) self))

(event EventEndPlay
  (params (EndPlayReason :type EEndPlayReason%20Enum :default "Destroyed"))
  (bind _asspyro_persistant_data (Utilities|Casting|CastToSpyro_PersistantData (Game|GetGameInstance)))
  (Utilities|Array|RemoveItem (Variables|/Game/SpyroContent/Global_Assets/Global_SaveData/Spyro_PersistantData.Spyro_PersistantData_C|GetAll_BlackPortals _asspyro_persistant_data) self))

(fn ConstructionScript)

(fn OnBlackPortalOverlap
  (params (Other%20Actor :type Object%20Object%20Reference) (Other%20Component :type Object%20Object%20Reference))
  (bind _staticmesh (Variables|Default|GetStaticMesh))
  (bind _returnvalue (Transformation|GetWorldLocation _staticmesh))
  (Variables|Default|GetPlayer_In_Portal
    (:then)
    (:else
      (bind _asbp_base_playable (Utilities|Casting|CastToBP_Base_Playable Other%20Actor))
      (if (Math|Boolean|ANDBoolean (== (Variables|/Script/Engine.Character|GetCapsuleComponent _asbp_base_playable) Other%20Component) (not (Utilities|Enum|Equal(Enum) (Variables|/Game/SpyroContent/Global_Assets/Global_Characters/Playable_Characters/BP_Base_Playable.BP_Base_Playable_C|GetPlayer_State _asbp_base_playable) "NewEnumerator11")) (Utilities|Enum|Equal(Enum) (Variables|/Game/SpyroContent/Global_Assets/Global_Components/Damageable_Com.Damageable_Com_C|GetDamage_Being_Taken (Variables|/Game/SpyroContent/Global_Assets/Global_Characters/Playable_Characters/BP_Base_Playable.BP_Base_Playable_C|GetDamageable _asbp_base_playable)) "NewEnumerator6"))
        (bind _sister_portal (Variables|Default|GetSister_Portal)
          (:then
            (bind _water_i_am_in (Variables|BP_BlackPortal_C|GetWater%20I%20Am%20In _sister_portal)
              (:then
                (Variables|/Game/SpyroContent/Global_Assets/Global_Characters/Playable_Characters/BP_Base_Playable.BP_Base_Playable_C|Setlatest%20water%20i%20entered _asbp_base_playable _water_i_am_in)
                (Variables|/Game/SpyroContent/Global_Assets/Global_Characters/Playable_Characters/BP_Base_Playable.BP_Base_Playable_C|SetEnvironmental_State _asbp_base_playable "NewEnumerator1"))
              (:else
                _))
            (CallFunction|Pause/UnpauseMusic Other%20Actor true false)
            (Variables|Default|SetPlayer_In_Portal _asbp_base_playable)
            (Variables|/Game/SpyroContent/Global_Assets/Global_Characters/Playable_Characters/BP_Base_Playable.BP_Base_Playable_C|SetMy%20Sublevel%20Index _asbp_base_playable (Variables|BP_BlackPortal_C|GetMy%20Sublevel%20Index (Variables|Default|GetSister_Portal)))
            (bind _asplayer_controller (Utilities|Casting|CastToPlayerController (Pawn|GetController (Variables|Default|GetPlayer_In_Portal)))
              (:then
                (Input|DisableInput (Variables|Default|GetPlayer_In_Portal) _asplayer_controller))
              (:CastFailed
                _))
            (bind _asbp_spyro (Utilities|Casting|CastToBP_Spyro (Variables|Default|GetPlayer_In_Portal))
              (:then
                (Variables|/Game/SpyroContent/Global_Assets/Global_Characters/Playable_Characters/Spyro/BP_Spyro.BP_Spyro_C|SetRight_DodgeRoll_Held _asbp_spyro false)
                (Variables|/Game/SpyroContent/Global_Assets/Global_Characters/Playable_Characters/Spyro/BP_Spyro.BP_Spyro_C|SetLeft_DodgeRoll_Held _asbp_spyro false)
                (bind _object_in_mouth (Variables|/Game/SpyroContent/Global_Assets/Global_Characters/Playable_Characters/Spyro/BP_Spyro.BP_Spyro_C|GetObject%20in%20Mouth _asbp_spyro)
                  (:then
                    (Default|ResetSpittableObject _object_in_mouth))
                  (:else
                    _)))
              (:CastFailed
                _))
            (Variables|/Game/SpyroContent/Global_Assets/Global_Characters/Playable_Characters/BP_Base_Playable.BP_Base_Playable_C|SetDid%20we%20disable%20input? (Variables|Default|GetPlayer_In_Portal) true)
            (Variables|/Game/SpyroContent/Global_Assets/Global_Characters/Playable_Characters/BP_Base_Playable.BP_Base_Playable_C|SetIn_BlackPortal_Transition (Variables|Default|GetPlayer_In_Portal) true)
            (Default|InvokedResetCamera (Variables|Default|GetPlayer_In_Portal))
            (Variables|/Game/SpyroContent/Global_Assets/Global_Characters/Playable_Characters/BP_Base_Playable.BP_Base_Playable_C|SetPlayer_State (Variables|Default|GetPlayer_In_Portal) "NewEnumerator0")
            (Components|Movement|StopMovementImmediately (Variables|/Script/Engine.Character|GetCharacterMovement (Variables|Default|GetPlayer_In_Portal)))
            (Character|StopJumping (Variables|Default|GetPlayer_In_Portal))
            (CallFunction|FadetoBlack)
            (if (Utilities|Enum|Equal(Enum) (Variables|/Game/SpyroContent/Global_Assets/Global_Characters/Playable_Characters/BP_Base_Playable.BP_Base_Playable_C|GetEnvironmental_State (Variables|Default|GetPlayer_In_Portal)) "NewEnumerator2")
              (Transformation|SetWorldLocation _staticmesh (Math|Vector|MakeVector (.x _returnvalue) (.y _returnvalue) (- (.z (Transformation|GetActorLocation (Variables|Default|GetPlayer_In_Portal))) (Variables|/Script/Engine.CapsuleComponent|GetCapsuleHalfHeight (Variables|/Script/Engine.Character|GetCapsuleComponent (Variables|Default|GetPlayer_In_Portal))))) false false)
              (Collision|SetCollisionEnabled (Variables|Default|GetStaticMesh) "QueryAndPhysics"))
            (Variables|/Game/SpyroContent/Global_Assets/Global_Characters/Playable_Characters/BP_Base_Playable.BP_Base_Playable_C|SetExit_BlackPortal (Variables|Default|GetPlayer_In_Portal) (select (Variables|Default|GetEntrance_Portal) (Variables|Default|GetSister_Portal) 0))
            (Default|CallPlayerEnteredBlackPortal)
            (bind _asspyro_player_controller (Utilities|Casting|CastToSpyro_PlayerController (Game|GetPlayerController 0)))
            (Default|HideAllQuestHUDs _asspyro_player_controller))
          (:else))))))