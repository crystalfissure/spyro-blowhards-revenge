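; Superflame fireball projectile that flies forward, deals super damage and explodes, or expires after a fixed lifetime.
; Tick moves it and sphere-traces for blockers, skipping an ignore list that varies for the Superfreeze subclass.
; Capsule overlaps and the one-shot blast trace share damage logic that depends on the creator and spares players talking to NPCs.
; Certain damage types on its Damageable hitbox extinguish it with smoke and a hiss.
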(event OnComponentBeginOverlap(Capsule)
  (params (OverlappedComponent :type Primitive%20Component%20Object%20Reference) (OtherActor :type Actor%20Object%20Reference) (OtherComp :type Primitive%20Component%20Object%20Reference) (OtherBodyIndex :type Integer) (bFromSweep :type Boolean) (SweepResult :type Hit%20Result%20Structure%20%28by%20ref%29))
  (CallFunction|DamageImpactTarget OtherActor OtherComp))

(event Custom|Delayed%20Self%20Destruct
  (params (Duration :type Float%20%28single-precision%29))
  (Utilities|FlowControl|Delay Duration)
  (Actor|DestroyActor))

(event Custom|Invoked%20Blow%20Up
  (bind _returnvalue (Transformation|GetActorLocation))
  (bind _returnvalue_2 (Transformation|GetActorLocation))
  (Utilities|FlowControl|DoOnce false
    (:Completed
      (Variables|Default|SetBlowing_Up true)
      (Components|Activation|Deactivate (Variables|Default|GetParticleSystem))
      (Rendering|SetVisibility (Variables|Default|GetStaticMesh) false false)
      (CallFunction|DelayedSelfDestruct (Variables|Default|GetExplosion%20Duration))
      (Effects|SpawnEmitteratLocation (Variables|Default|GetBlast_Type) _returnvalue (Math|Rotator|MakeRotator 0.0 0.0 (- (.yaw (Transformation|GetWorldRotation (Variables|Default|GetStaticMesh))) 9e+01)))
      (Audio|PlaySoundatLocation (Variables|Default|GetImpact%20SFX) _returnvalue "0, 0, 0" 1.0 1.0 0.0 0 0 0)
      (bind _outhits (Collision|MultiSphereTraceForObjects _returnvalue_2 _returnvalue_2 (Variables|Default|GetExplosion%20Radius) (Utilities|Array|MakeArray "ObjectTypeQuery1" "ObjectTypeQuery2" "ObjectTypeQuery3" "ObjectTypeQuery8" "ObjectTypeQuery9") false 0 "None"))
      (for _array_element _outhits
        (CallFunction|DamageImpactTarget (.hitactor _array_element) (.hitcomponent _array_element))))))

(event Custom|Damage%20Impact%20Target
  (params (Other%20Actor :type Actor%20Object%20Reference) (Other%20Comp :type Actor%20Component%20Object%20Reference))
  (bind _returnvalue (Actor|GetComponentbyClass Other%20Actor "/Game/SpyroContent/Global_Assets/Global_Components/Damageable_Com.Damageable_Com_C"))
  (bind _particlesystem (Variables|Default|GetParticleSystem))
  (bind _returnvalue_2 (Math|Vector|GetForwardVector _particlesystem))
  (bind _object_s_hitbox_component (Variables|/Game/SpyroContent/Global_Assets/Global_Components/Damageable_Com.Damageable_Com_C|GetObject's%20Hitbox%20Component _returnvalue))
  (bind _returnvalue_3 (== _object_s_hitbox_component Other%20Comp))
  (Utilities|IsValid Other%20Actor
    (:Is%20Valid
      (Utilities|IsValid _returnvalue
        (:Is%20Valid
          (bind _my_creator (Variables|Default|GetMy_Creator)
            (:then
              (bind _asbase_enemy_bp (Utilities|Casting|CastToBase_Enemy_BP _my_creator)
                (:then
                  (if (and (not (Utilities|Enum|Equal(Enum) (Variables|/Game/SpyroContent/Global_Assets/Global_Components/Base_AI_Character.Base_AI_Character_C|GetAICharacter_State (Variables|/Game/SpyroContent/Global_Assets/Global_Characters/AI_Characters/Actors/Base_AICharacter_BP.Base_AICharacter_BP_C|GetWalking_AI_Character _asbase_enemy_bp)) "NewEnumerator3")) (and _returnvalue_3 (not (== _my_creator Other%20Actor))))
                    (bind _asbp_base_playable (Utilities|Casting|CastToBP_Base_Playable Other%20Actor)
                      (:then
                        (Variables|/Game/SpyroContent/Global_Assets/Global_Characters/Playable_Characters/BP_Base_Playable.BP_Base_Playable_C|GetTalking_NPC _asbp_base_playable
                          (:then
                            _)
                          (:else
                            (Utilities|FlowControl|DoOnce false
                              (:Completed
                                (Default|DealDamage _returnvalue (Variables|Default|GetDamage%20Type) _returnvalue_2 true (Variables|Default|GetMy_Creator) false :!label _label))))))
                      (:CastFailed
                        (goto _label)))
                    (CallFunction|InvokedBlowUp)))
                (:CastFailed
                  (if (and _returnvalue_3 (not (== _my_creator Other%20Actor)))
                    (Default|DealDamage _returnvalue (Variables|Default|GetDamage%20Type) _returnvalue_2 true (Variables|Default|GetMy_Creator) false)
                    (bind _superflame_ignores_this (CallFunction|DoesSuperflameIgnoreThis? Other%20Actor))
                    (if (not _superflame_ignores_this)
                      (CallFunction|InvokedBlowUp))))))
            (:else
              (if (and _returnvalue_3 (Variables|Default|GetNo%20Creator))
                (bind _asbp_base_playable_2 (Utilities|Casting|CastToBP_Base_Playable Other%20Actor)
                  (:then
                    (Variables|/Game/SpyroContent/Global_Assets/Global_Characters/Playable_Characters/BP_Base_Playable.BP_Base_Playable_C|GetTalking_NPC _asbp_base_playable_2
                      (:then
                        _)
                      (:else
                        (Utilities|FlowControl|DoOnce false
                          (:Completed
                            (Default|DealDamage _returnvalue (Variables|Default|GetDamage%20Type) _returnvalue_2 true 0 false :!label _label_2))))))
                  (:CastFailed
                    (goto _label_2)))
                (CallFunction|InvokedBlowUp)))))))))

(event Custom|Extinguish%20Fireball?
  (bind _returnvalue (Transformation|GetActorLocation))
  (bind _damageable_comp (Variables|Default|GetDamageable_Comp))
  (bind _deal_damage___damage_type (Variables|/Game/SpyroContent/Global_Assets/Global_Components/Damageable_Com.Damageable_Com_C|GetDeal%20Damage%20-%20Damage%20Type _damageable_comp))
  (if (Math|Boolean|ORBoolean (Utilities|Enum|Equal(Enum) _deal_damage___damage_type "NewEnumerator11") (Utilities|Enum|Equal(Enum) _deal_damage___damage_type "NewEnumerator7") (Utilities|Enum|Equal(Enum) _deal_damage___damage_type "NewEnumerator10") (Utilities|Enum|Equal(Enum) _deal_damage___damage_type "NewEnumerator12") (Utilities|Enum|Equal(Enum) _deal_damage___damage_type "NewEnumerator13"))
    (Audio|PlaySoundatLocation "/Game/SpyroContent/Global_Assets/Global_Level_Items/Treasure_Containers/Fire_Container/fire_extinguished_hiss.fire_extinguished_hiss" _returnvalue "0, 0, 0" 1.0 1.0 0.0 0 0 0)
    (Effects|SpawnEmitteratLocation "/Game/SpyroContent/Global_Assets/Global_Level_Items/Dragon_Breath/Particles/smoke_wafting.smoke_wafting" _returnvalue)
    (Actor|DestroyActor)))

(event EventBeginPlay
  (Variables|/Game/SpyroContent/Global_Assets/Global_Components/Damageable_Com.Damageable_Com_C|SetObject's%20Hitbox%20Component (Variables|Default|GetDamageable_Comp) (Variables|Default|Getextinguish%20hitbox))
  (EventDispatchers|BindEventtoCallDealDamage (Variables|Default|GetDamageable_Comp) (delegate Custom|Extinguish%20Fireball?))
  (Utilities|FlowControl|Delay 1e+01)
  (Actor|DestroyActor))

(event EventTick
  (params (DeltaSeconds :type Float%20%28single-precision%29))
  (if (not (Variables|Default|GetBlowing_Up))
    (Utilities|FlowControl|Sequence
      (:then_0
        (CallFunction|SphereTrace (Transformation|GetActorRightVector) "None" 2e+01))
      (:then_1
        (Transformation|AddActorWorldOffset (* (Math|Vector|GetForwardVector (Variables|Default|GetParticleSystem)) (* DeltaSeconds (Variables|Default|GetSpeed))))))))

(fn ConstructionScript)

(fn SphereTrace
  (params (Vector :type Vector) (DrawDebugType :type EDrawDebugTrace%20Enum :default "None") (Trace%20Length :type Float%20%28single-precision%29))
  (bind _returnvalue (Transformation|GetActorLocation))
  (bind _outhits (Collision|MultiSphereTraceForObjects _returnvalue (+ _returnvalue (* Vector Trace%20Length)) (Variables|Default|GetInitial%20Radius) (Utilities|Array|MakeArray "ObjectTypeQuery1" "ObjectTypeQuery2" "ObjectTypeQuery3" "ObjectTypeQuery8" "ObjectTypeQuery9") false 0 DrawDebugType))
  (bind _array_element (Utilities|Array|ForEachLoopwithBreak _outhits :!label _label)
    (:LoopBody
      (if (.bblockinghit _array_element)
        (bind _my_creator (Variables|Default|GetMy_Creator)
          (:then
            (if (not (== _my_creator (.hitactor _array_element)))
              (bind _superflame_ignores_this (CallFunction|DoesSuperflameIgnoreThis? (.hitactor _array_element) :!label _label_2))
              (if (not _superflame_ignores_this)
                (CallFunction|InvokedBlowUp)
                (goto _label Break))))
          (:else
            (goto _label_2)))))
    (:Completed
      (return (.hitactor _array_element) (.hitcomponent _array_element)))))

(fn DoesSuperflameIgnoreThis?
  (params (Object :type Object%20Object%20Reference))
  (Utilities|FlowControl|Sequence
    (:then_0
      (Utilities|IsValid Object
        (:Is%20Valid
          (Utilities|Casting|CastToSuperflame_BP Object
            (:then
              _)
            (:CastFailed
              (Utilities|Casting|CastToGem_Base_BP Object
                (:then
                  _)
                (:CastFailed
                  (Utilities|Casting|CastToSparx_BP Object
                    (:then
                      _)
                    (:CastFailed
                      (Utilities|Casting|CastToBouncing_Numbers_BP Object
                        (:then
                          _)
                        (:CastFailed
                          (Utilities|Casting|CastToGold_Text Object
                            (:then
                              _)
                            (:CastFailed
                              (Utilities|Casting|CastToBasket_BP Object
                                (:then
                                  _)
                                (:CastFailed
                                  (Utilities|Casting|CastToVase_BP Object
                                    (:then
                                      (Utilities|Casting|CastToSuperfreeze_BP self
                                        (:then
                                          (Utilities|Casting|CastToButterfly_Jar_BP Object :!label _label
                                            (:then
                                              _)
                                            (:CastFailed
                                              (Utilities|Casting|CastToSheep_BP Object
                                                (:then
                                                  _)
                                                (:CastFailed
                                                  (bind _asactor (Utilities|Casting|CastToActor Object))
                                                  (Utilities|IsValid (Actor|GetComponentbyClass _asactor "/Game/SpyroContent/Global_Assets/Global_Components/DragonBreath_Damages_Me_Without_Getting_Blocked.DragonBreath_Damages_Me_Without_Getting_Blocked_C")
                                                    (:Is%20Valid
                                                      _)))))))
                                        (:CastFailed
                                          _)))
                                    (:CastFailed
                                      (goto _label)))))))))))))))
          (LocalVariables|SetSuperflame_Ignores_This true))))
    (:then_1
      (return (LocalVariables|GetSuperflame_Ignores_This)))))