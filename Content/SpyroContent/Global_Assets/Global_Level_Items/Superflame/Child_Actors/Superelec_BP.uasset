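; Superelec_BP is the electric Superflame child actor that electrifies swimmable water when it blows up.
; InvokedBlowUp sphere-traces for objects at ExtinguishHitbox, using three times its capsule radius, and calls ElectrifyWater on the Swimmable_Water_BP actors it hits.
; If the creator is a playable character, that player is first marked as immune on the water.
; The parent's blow-up logic runs after the trace loop.
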(event EventBeginPlay
  (|CallParentFunction) ; This node is disabled and will not be called.\nDrag off pins to build functionality.
)

(event Collision|EventActorBeginOverlap
  (params (OtherActor :type Actor%20Object%20Reference)))

(event EventTick
  (params (DeltaSeconds :type Float%20%28single-precision%29))
  (|CallParentFunction DeltaSeconds) ; This node is disabled and will not be called.\nDrag off pins to build functionality.
)

(event EventInvokedBlowUp
  (bind _extinguish_hitbox (Variables|Default|Getextinguish%20hitbox))
  (bind _returnvalue (Transformation|GetWorldLocation _extinguish_hitbox))
  (bind _outhits (Collision|MultiSphereTraceForObjects _returnvalue _returnvalue (* (Variables|/Script/Engine.CapsuleComponent|GetCapsuleRadius _extinguish_hitbox) 3.0) (Utilities|Array|MakeArray "ObjectTypeQuery7") false 0 "None"))
  (bind _array_element (Utilities|Array|ForEachLoopwithBreak _outhits)
    (:LoopBody
      (if (.bblockinghit _array_element)
        (bind _asswimmable_water_bp (Utilities|Casting|CastToSwimmable_Water_BP (.hitactor _array_element)))
        (bind _asbp_base_playable (Utilities|Casting|CastToBP_Base_Playable (Variables|Default|GetMy_Creator))
          (:then
            (Variables|/Game/SpyroContent/Global_Assets/Global_Level_Items/Swimmable_Water/Actors/Swimmable_Water_BP.Swimmable_Water_BP_C|Setplayer%20who%20cannot%20be%20electrified _asswimmable_water_bp _asbp_base_playable))
          (:CastFailed
            _))
        (Default|ElectrifyWater _asswimmable_water_bp)))
    (:Completed
      (|CallParentFunction))))

(fn ConstructionScript
  (|CallParentFunction))