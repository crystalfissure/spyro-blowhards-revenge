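; Superfreeze actor, filed under the Superflame child actors, that lays ice on water beneath it.
; Each tick it line-traces 100 units straight down against world static and one other object type.
; When the hit actor is swimmable or drownable water, it spawns an IceHex_BP slightly above the impact location, with no check for existing hexes.
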(event EventBeginPlay
  (|CallParentFunction) ; This node is disabled and will not be called.\nDrag off pins to build functionality.
)

(event Collision|EventActorBeginOverlap
  (params (OtherActor :type Actor%20Object%20Reference)))

(event EventTick
  (params (DeltaSeconds :type Float%20%28single-precision%29))
  (bind _returnvalue (Transformation|GetActorLocation))
  (bind (_x _y _z) (Math|Vector|BreakVector _returnvalue))
  (|CallParentFunction DeltaSeconds)
  (bind _outhit (Collision|LineTraceForObjects _returnvalue (Math|Vector|MakeVector _x _y (- _z 1e+02)) (Utilities|Array|MakeArray "ObjectTypeQuery1" "ObjectTypeQuery10") false 0 "None"))
  (if (.bblockinghit _outhit)
    (Utilities|Casting|CastToSwimmable_Water_BP (.hitactor _outhit)
      (:then
        _)
      (:CastFailed
        (Utilities|Casting|CastToDrownable_Water_BP (.hitactor _outhit))))
    (Game|SpawnActorfromClass "/Game/SpyroContent/Global_Assets/Global_Level_Items/Ice_Skating/IceHex_BP.IceHex_BP_C" (Math|Transform|MakeTransform (Math|Vector|MakeVector (.X (Math|Vector|BreakVector (.location _outhit))) (.Y (Math|Vector|BreakVector (.location _outhit))) (+ (.Z (Math|Vector|BreakVector (.location _outhit))) 15.0)) "0, 0, 0" "1,1,1") "AlwaysSpawn" 0 0)))

(fn ConstructionScript
  (|CallParentFunction))