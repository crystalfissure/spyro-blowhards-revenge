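; Green sphere child actor in the Superflame item set that moves vertically until it starts blowing up.
; A timeline started on BeginPlay sets GoingDownAmount, which scales a frame-rate-independent vertical world offset each tick after the parent's tick.
; While not BlowingUp, it also runs a short SphereTrace down its local up axis after each move.
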(event EventBeginPlay
  (bind _newtrack_0 (Timeline|Timeline_0 PlayFromStart)
    (:Update
      (Variables|Default|SetGoing%20Down%20Amount _newtrack_0))))

(event EventTick
  (params (DeltaSeconds :type Float%20%28single-precision%29))
  (|CallParentFunction DeltaSeconds)
  (if (not (Variables|Default|GetBlowing_Up))
    (Transformation|AddActorWorldOffset (Math|Vector|MakeVector 0.0 0.0 (* DeltaSeconds 2e+02 (Variables|Default|GetGoing%20Down%20Amount))))
    (CallFunction|SphereTrace (Transformation|GetActorUpVector) "None" -2e+01)))

(fn ConstructionScript
  (|CallParentFunction))