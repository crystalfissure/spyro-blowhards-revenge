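; Destructible actor in the global level items that breaks apart as soon as play begins for it.
; On BeginPlay its Destructible component applies full radius damage to itself at its own location, using configurable damage, radius and impulse.
; Unless LastsForever is set, the actor destroys itself after a Duration delay.
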(event EventBeginPlay
  (bind _destructible (Variables|Default|GetDestructible))
  (Class|DestructibleComponent|ApplyRadiusDamage _destructible (Variables|Default|GetBase%20Damage) (Transformation|GetWorldLocation _destructible) (Variables|Default|GetDamage%20Radius) (Variables|Default|GetImpulse%20Strength) true)
  (if (not (Variables|Default|GetLasts_Forever))
    (Utilities|FlowControl|Delay (Variables|Default|GetDuration))
    (Actor|DestroyActor)))

(fn ConstructionScript)