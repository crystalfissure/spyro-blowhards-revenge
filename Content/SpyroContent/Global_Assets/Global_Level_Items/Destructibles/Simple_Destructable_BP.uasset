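; Simple breakable prop that shatters when hit by damage it is not resistant to, or by super damage unless the Damageable component ignores it.
; The Damageable component uses the Box as its hitbox and calls OnDamaged, which checks the damage requirement.
; A passing hit runs once: it confirms the damage, plays a sound, hides the mesh, spawns a Basket_Burst_BP shard burst, then destroys the actor shortly after.
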(event Custom|On%20Damaged
  (bind _returnvalue (CallFunction|DamageRequirement))
  (if _returnvalue
    (Utilities|FlowControl|DoOnce false
      (:Completed
        (Default|CallDamageWasSuccessfullyDealt (Variables|Default|GetDamageable))
        (Audio|PlaySoundatLocation (Variables|Default|Getdestroyed%20sound) (Transformation|GetWorldLocation (Variables|Default|GetShrapnel%20&%20Sound%20Origin)) "0, 0, 0" 1.0 1.0 0.0 0 0 0)
        (Rendering|SetActorHiddenInGame true)
        (Collision|SetCollisionResponsetoAllChannels (Variables|Default|GetStaticMesh) "ECR_Ignore")
        (bind _returnvalue_2 (Game|SpawnActorfromClass "/Game/SpyroContent/Global_Assets/Global_Level_Items/Treasure_Containers/Basket/Actors/Basket_Burst_BP.Basket_Burst_BP_C" (Transformation|GetWorldTransform (Variables|Default|GetShrapnel%20&%20Sound%20Origin)) "AdjustIfPossibleButAlwaysSpawn" 0 0))
        (Default|ShardBurstAction _returnvalue_2 (Variables|Default|GetShard%20Mesh%201) (Variables|Default|GetShard%20Mesh%202))
        (Utilities|FlowControl|Delay 0.2)
        (Actor|DestroyActor)))))

(event EventBeginPlay
  (Variables|/Game/SpyroContent/Global_Assets/Global_Components/Damageable_Com.Damageable_Com_C|SetObject's%20Hitbox%20Component (Variables|Default|GetDamageable) (Variables|Default|GetBox))
  (EventDispatchers|BindEventtoCallDealDamage (Variables|Default|GetDamageable) (delegate Custom|On%20Damaged)))

(fn ConstructionScript)

(fn AmIResistanttoThis?
  (LocalVariables|Setim%20resistant false)
  (bind _array_element (Utilities|Array|ForEachLoopwithBreak (Variables|/Game/SpyroContent/Global_Assets/Global_Components/Damageable_Com.Damageable_Com_C|GetDamage_Resistances (Variables|Default|GetDamageable)) :!label _label)
    (:LoopBody
      (if (Utilities|Enum|Equal(Enum) _array_element (Variables|/Game/SpyroContent/Global_Assets/Global_Components/Damageable_Com.Damageable_Com_C|GetDeal%20Damage%20-%20Damage%20Type (Variables|Default|GetDamageable)))
        (LocalVariables|Setim%20resistant true)
        (goto _label Break)))
    (:Completed
      (return (LocalVariables|Getim%20resistant)))))

(fn DamageRequirement
  (bind _im_resistant_ (CallFunction|AmIResistanttoThis?))
  (return (or (and (Variables|/Game/SpyroContent/Global_Assets/Global_Components/Damageable_Com.Damageable_Com_C|GetDeal%20Damage%20-%20Super%20Damage (Variables|Default|GetDamageable)) (not (Variables|/Game/SpyroContent/Global_Assets/Global_Components/Damageable_Com.Damageable_Com_C|GetIgnore%20If%20Super%20or%20Not (Variables|Default|GetDamageable)))) (not _im_resistant_))))