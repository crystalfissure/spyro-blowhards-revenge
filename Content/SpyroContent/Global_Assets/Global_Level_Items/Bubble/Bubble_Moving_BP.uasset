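; Moving Spyro bubble that grows as it travels, acts as a hurlwind that flings the player outside Superfly, and pops after a few seconds.
; Repeated midair breaths shrink its size and launch strength and change its timeline-driven speed.
; A looping sphere trace ignores players, bubbles, butterflies and gems, damages Damageable components, then generally pops the bubble or, on static world geometry, makes it drift slowly backward.
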(event EventBeginPlay
  (bind _returnvalue (Math|Float|MakeLiteralFloat 5e+02))
  (bind _times_player_breathed_in_air (Variables|Default|GetTimes%20Player%20Breathed%20in%20Air))
  (bind _times_player_breathed_in_air_2 (Variables|Default|GetTimes%20Player%20Breathed%20in%20Air))
  (bind _times_player_breathed_in_air_3 (Variables|Default|GetTimes%20Player%20Breathed%20in%20Air))
  (bind _times_player_breathed_in_air_4 (Variables|Default|GetTimes%20Player%20Breathed%20in%20Air))
  (bind _returnvalue_2 (<= _times_player_breathed_in_air 0))
  (bind _returnvalue_3 (>= _times_player_breathed_in_air_2 4))
  (bind _returnvalue_4 (Utilities|Select :Index _times_player_breathed_in_air_2 :Option%200 1.0 :Option%201 0.7 :Option%202 0.55 :Option%203 0.4))
  (bind _returnvalue_5 (select _returnvalue_3 0.4 _returnvalue_4))
  (|CallParentFunction)
  (Variables|Default|SetLaunch%20Velocity%20Z (* (Variables|Default|GetLaunch%20Velocity%20Z) (select (>= _times_player_breathed_in_air_3 4) 0.7 (Utilities|Select :Index _times_player_breathed_in_air_3 :Option%200 1.0 :Option%201 0.9 :Option%202 0.8 :Option%203 0.7))))
  (Utilities|Time|SetTimerbyFunctionName 0 "Col Ping" 0.1 true)
  (Utilities|FlowControl|Sequence
    (:then_0
      (bind _newtrack_0 (Timeline|Timeline_0 PlayFromStart)
        (:Update
          (Transformation|SetActorScale3D (Math|Vector|Lerp(Vector) "0.100000,0.100000,0.100000" (select _returnvalue_2 "1.000000,1.000000,1.000000" (Math|Vector|MakeVector _returnvalue_5 _returnvalue_5 _returnvalue_5)) _newtrack_0)))
        (:Finished
          (if _returnvalue_2
            (Rendering|SetVisibility (Variables|Default|GetMaterialBillboard) true false)))))
    (:then_1
      (Utilities|FlowControl|Delay 0.2)
      (CallFunction|ToggleHurlwind true)
      (Utilities|FlowControl|Sequence
        (:then_0
          (bind _newtrack_0_2 (Timeline|Timeline_1 PlayFromStart)
            (:Update
              (Variables|Default|SetSpeed (select (Variables|Default|Getdouble%20max%20speed) 3e+03 (select (Variables|Default|GetMax%20Speed) 1e+03 (Math|Float|Lerp 1e+03 (select (>= _times_player_breathed_in_air_4 4) _returnvalue (Utilities|Select :Index _times_player_breathed_in_air_4 :Option%200 1e+02 :Option%201 2e+02 :Option%202 3e+02 :Option%203 _returnvalue)) _newtrack_0_2)))))))
        (:then_1
          (Utilities|FlowControl|Delay 0.3)
          (Variables|Default|SetBubble%20at%20full%20size true)
          (Utilities|FlowControl|Delay 5.0)
          (CallFunction|PopBubble))))))

(event EventFlingPlayer
  (params (Other%20Actor :type Object%20Object%20Reference) (Other%20Comp :type Object%20Object%20Reference))
  (bind _asbp_spyro (Utilities|Casting|CastToBP_Spyro Other%20Actor))
  (if (not (> (Variables|/Game/SpyroContent/Global_Assets/Global_Characters/Playable_Characters/Spyro/BP_Spyro.BP_Spyro_C|GetSuperfly_Speedup _asbp_spyro) 0.0))
    (|CallParentFunction Other%20Actor Other%20Comp)))

(event EventTick
  (params (DeltaSeconds :type Float%20%28single-precision%29))
  (bind _speed (Variables|Default|GetSpeed))
  (Transformation|AddActorWorldOffset (* (* (Math|Vector|GetForwardVector (Variables|Default|GetArrow)) DeltaSeconds) (select (Variables|Default|Getfreeze%20in%20place) (* _speed -0.1) _speed))))

(fn ConstructionScript
  (|CallParentFunction))

(fn ColPing
  (bind _returnvalue (Transformation|GetActorRotation))
  (bind _outhits (Collision|MultiSphereTraceForObjects (+ (Transformation|GetActorLocation) (* (Transformation|GetActorUpVector) 2e+01)) (+ (Transformation|GetActorLocation) (* (Math|Vector|GetForwardVector (Math|Rotator|MakeRotator (.roll _returnvalue) (.pitch _returnvalue) (+ (.yaw _returnvalue) 9e+01))) 5e+01) (* (Transformation|GetActorUpVector) 2e+01)) 3e+01 (Utilities|Array|MakeArray "ObjectTypeQuery1" "ObjectTypeQuery2" "ObjectTypeQuery3") false 0 "None"))
  (bind _array_element (Utilities|Array|ForEachLoopwithBreak _outhits :!label _label)
    (:LoopBody
      (Utilities|IsValid (.hitactor _array_element)
        (:Is%20Valid
          (if (.bblockinghit _array_element)
            (Utilities|Casting|CastToBP_Base_Playable (.hitactor _array_element)
              (:CastFailed
                (Utilities|Casting|CastToBubble_BP (.hitactor _array_element)
                  (:CastFailed
                    (Utilities|Casting|CastToButterfly_BP (.hitactor _array_element)
                      (:CastFailed
                        (Utilities|Casting|CastToGem_Base_BP (.hitactor _array_element)
                          (:CastFailed
                            (Utilities|IsValid (Actor|GetComponentbyClass (.hitactor _array_element) "/Game/SpyroContent/Global_Assets/Global_Components/Damageable_Com.Damageable_Com_C")
                              (:Is%20Valid
                                (Default|DealDamage (Actor|GetComponentbyClass (.hitactor _array_element) "/Game/SpyroContent/Global_Assets/Global_Components/Damageable_Com.Damageable_Com_C") "NewEnumerator10" "0, 0, 0" false 0 false))
                              (:Is%20Not%20Valid
                                _))
                            (Variables|Default|SetActive true)
                            (Utilities|IsValid (Actor|GetComponentbyClass (.hitactor _array_element) "/Game/SpyroContent/Global_Assets/Global_Components/DragonBreath_Damages_Me_Without_Getting_Blocked.DragonBreath_Damages_Me_Without_Getting_Blocked_C")
                              (:Is%20Valid
                                (goto _label Break))
                              (:Is%20Not%20Valid
                                (if (Utilities|Enum|Equal(Enum) (Collision|GetCollisionObjectType (.hitcomponent _array_element)) "ECC_WorldStatic")
                                  (Utilities|Casting|CastToTreasure_Container_Base_BP (.hitactor _array_element)
                                    (:then
                                      _)
                                    (:CastFailed
                                      (Variables|Default|Setfreeze%20in%20place true)
                                      (goto _label Break))))
                                (CallFunction|PopBubble)
                                (goto _label Break)))))))))))))
        (:Is%20Not%20Valid
          (Variables|Default|Setfreeze%20in%20place true))))))