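; Poppable bubble that flings the player, built on a parent fling actor with a toggleable whirlwind.
; Damage from all but one type pops an active bubble, playing a sound and switching off the whirlwind.
; Flinging works only at full size, then joins the pop logic past the sound, with a shorter respawn delay.
; The bubble hides with a particle burst, then either reappears or destroys itself, depending on its respawn flag.
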(event Custom|pop%20bubble
  (bind _returnvalue (Transformation|GetActorLocation))
  (bind _returnvalue_2 (Transformation|GetActorLocation))
  (if (Math|Boolean|ANDBoolean (not (Variables|Default|Getpopped)) (not (Utilities|Enum|Equal(Enum) (Variables|/Game/SpyroContent/Global_Assets/Global_Components/Damageable_Com.Damageable_Com_C|GetDeal%20Damage%20-%20Damage%20Type (Variables|Default|GetDamageable_Comp)) "NewEnumerator4")) (Variables|Default|GetActive))
    (Variables|Default|Setpopped true)
    (CallFunction|ToggleHurlwind false)
    (Audio|PlaySoundatLocation "/Game/SpyroContent/Global_Assets/Global_Level_Items/Bubble/Pop2.Pop2" (Transformation|GetActorLocation) "0, 0, 0" 1.0 1.0 0.0 0 0 0)
    (if (Variables|Default|GetRespaws)
      (Rendering|SetActorHiddenInGame true)
      (Effects|SpawnEmitteratLocation "/Game/SpyroContent/Global_Assets/Global_Level_Items/Bubble/bubble_pop_particle.bubble_pop_particle" (Math|Vector|MakeVector (.x _returnvalue) (.y _returnvalue) (+ (.z _returnvalue) 5e+01)))
      (Utilities|FlowControl|Delay (select (Variables|Default|Getpopped) 1.0 0.5))
      (Rendering|SetActorHiddenInGame false)
      (Variables|Default|Setpopped false)
      (CallFunction|ToggleHurlwind true)
      (else
        (Variables|Default|SetActive false)
        (Rendering|SetActorHiddenInGame true)
        (Effects|SpawnEmitteratLocation "/Game/SpyroContent/Global_Assets/Global_Level_Items/Bubble/bubble_pop_particle.bubble_pop_particle" (Math|Vector|MakeVector (.x _returnvalue_2) (.y _returnvalue_2) (+ (.z _returnvalue_2) 5e+01)))
        (Utilities|FlowControl|Delay 1.0)
        (Actor|DestroyActor)))))

(event EventBeginPlay
  (bind _damageable_comp (Variables|Default|GetDamageable_Comp))
  (|CallParentFunction)
  (Variables|/Game/SpyroContent/Global_Assets/Global_Components/Damageable_Com.Damageable_Com_C|SetObject's%20Hitbox%20Component _damageable_comp (Variables|Default|GetBox))
  (EventDispatchers|BindEventtoCallDealDamage _damageable_comp (delegate Custom|pop%20bubble)))

(event EventFlingPlayer
  (params (Other%20Actor :type Object%20Object%20Reference) (Other%20Comp :type Object%20Object%20Reference))
  (bind _returnvalue (Transformation|GetActorLocation))
  (bind _returnvalue_2 (Transformation|GetActorLocation))
  (if (Variables|Default|GetBubble%20at%20full%20size)
    (|CallParentFunction Other%20Actor Other%20Comp)
    (bind _asbp_base_playable (Utilities|Casting|CastToBP_Base_Playable Other%20Actor))
    (if (== (Variables|/Script/Engine.Character|GetCapsuleComponent _asbp_base_playable) Other%20Comp)
      (bind _fling_player_ (CallFunction|FlingPlayerConditions _asbp_base_playable (Variables|/Script/Engine.Character|GetCapsuleComponent _asbp_base_playable)))
      (if _fling_player_
        (if (Variables|Default|GetRespaws)
          (Rendering|SetActorHiddenInGame true)
          (Effects|SpawnEmitteratLocation "/Game/SpyroContent/Global_Assets/Global_Level_Items/Bubble/bubble_pop_particle.bubble_pop_particle" (Math|Vector|MakeVector (.x _returnvalue) (.y _returnvalue) (+ (.z _returnvalue) 5e+01)))
          (Utilities|FlowControl|Delay (select (Variables|Default|Getpopped) 1.0 0.5))
          (Rendering|SetActorHiddenInGame false)
          (Variables|Default|Setpopped false)
          (CallFunction|ToggleHurlwind true)
          (else
            (Variables|Default|SetActive false)
            (Rendering|SetActorHiddenInGame true)
            (Effects|SpawnEmitteratLocation "/Game/SpyroContent/Global_Assets/Global_Level_Items/Bubble/bubble_pop_particle.bubble_pop_particle" (Math|Vector|MakeVector (.x _returnvalue_2) (.y _returnvalue_2) (+ (.z _returnvalue_2) 5e+01)))
            (Utilities|FlowControl|Delay 1.0)
            (Actor|DestroyActor)))))))

(fn ConstructionScript
  (|CallParentFunction))