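; Drownable water volume that harms playable characters whose capsule enters its hitbox, with the collision component copying the hitbox mesh at BeginPlay.
; Unless invincible, the player changes state, stops, normally loses one hit point, dies at zero and incurs a skill-level penalty.
; An experimental flag instead teleports Spyro to a speedway start.
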(event OnComponentBeginOverlap(Hitbox)
  (params (OverlappedComponent :type Primitive%20Component%20Object%20Reference) (OtherActor :type Actor%20Object%20Reference) (OtherComp :type Primitive%20Component%20Object%20Reference) (OtherBodyIndex :type Integer) (bFromSweep :type Boolean) (SweepResult :type Hit%20Result%20Structure%20%28by%20ref%29))
  (CallFunction|DrownthePlayer OtherActor OtherComp))

(event EventBeginPlay
  (Components|StaticMesh|SetStaticMesh (Variables|Default|GetCollision) (Variables|/Script/Engine.StaticMeshComponent|GetStaticMesh (Variables|Default|GetHitbox))))

(fn ConstructionScript)

(fn DrownthePlayer
  (params (Other%20Actor :type Object%20Object%20Reference) (Other%20Comp :type Object%20Object%20Reference))
  (bind _asbp_base_playable (Utilities|Casting|CastToBP_Base_Playable Other%20Actor))
  (if (and (== (Variables|/Script/Engine.Character|GetCapsuleComponent _asbp_base_playable) Other%20Comp) (not (Utilities|Enum|Equal(Enum) (Variables|/Game/SpyroContent/Global_Assets/Global_Characters/Playable_Characters/BP_Base_Playable.BP_Base_Playable_C|GetPlayer_State _asbp_base_playable) "NewEnumerator11")))
    ;[0.207 0.03193 0.5573] qtderg experimental modification
    ;
    ; Teleporting to a speedway start
    (if (Variables|Default|GetTeleport%20to%20a%20speedway)
      (bind _asbp_spyro (Utilities|Casting|CastToBP_Spyro _asbp_base_playable))
      (Default|TeleporttoSpeedway _asbp_spyro)
      (else
        (if (Utilities|Enum|Equal(Enum) (Variables|/Game/SpyroContent/Global_Assets/Global_Characters/Playable_Characters/BP_Base_Playable.BP_Base_Playable_C|GetEnvironmental_State _asbp_base_playable) "NewEnumerator1")
          (Variables|/Game/SpyroContent/Global_Assets/Global_Characters/Playable_Characters/BP_Base_Playable.BP_Base_Playable_C|SetEnvironmental_State _asbp_base_playable "NewEnumerator0")
          (Transformation|SetActorRotation _asbp_base_playable (Math|Rotator|MakeRotator 0.0 0.0 (.yaw (Transformation|GetActorRotation _asbp_base_playable)))))
        (Variables|/Game/SpyroContent/Global_Assets/Global_Characters/Playable_Characters/BP_Base_Playable.BP_Base_Playable_C|SetGround_State _asbp_base_playable "NewEnumerator5")
        (if (Math|Boolean|ANDBoolean (not (Utilities|Enum|Equal(Enum) (Variables|/Game/SpyroContent/Global_Assets/Global_Characters/Playable_Characters/BP_Base_Playable.BP_Base_Playable_C|GetPlayer_State _asbp_base_playable) "NewEnumerator22")) (not (Variables|/Game/SpyroContent/Global_Assets/Global_Characters/Playable_Characters/BP_Base_Playable.BP_Base_Playable_C|GetCHEAT_Invincibility _asbp_base_playable)) (not (Variables|/Game/SpyroContent/Global_Assets/Global_Characters/Playable_Characters/BP_Base_Playable.BP_Base_Playable_C|GetSuperinvincibility _asbp_base_playable)) (not (Variables|/Game/SpyroContent/Global_Assets/Global_Components/Damageable_Com.Damageable_Com_C|GetInvincible (Variables|/Game/SpyroContent/Global_Assets/Global_Characters/Playable_Characters/BP_Base_Playable.BP_Base_Playable_C|GetDamageable _asbp_base_playable))))
          (Variables|/Game/SpyroContent/Global_Assets/Global_Characters/Playable_Characters/BP_Base_Playable.BP_Base_Playable_C|SetPlayer_State _asbp_base_playable "NewEnumerator22")
          (Components|Movement|StopMovementImmediately (Variables|/Script/Engine.Character|GetCharacterMovement _asbp_base_playable))
          (bind _output_get (Variables|/Game/SpyroContent/Global_Assets/Global_Components/Damageable_Com.Damageable_Com_C|SetHit%20Points (Variables|/Game/SpyroContent/Global_Assets/Global_Characters/Playable_Characters/BP_Base_Playable.BP_Base_Playable_C|GetDamageable _asbp_base_playable) (select (Utilities|Enum|Equal(Enum) (Variables|/Game/SpyroContent/Global_Assets/Global_Characters/Playable_Characters/BP_Base_Playable.BP_Base_Playable_C|GetSparxLimit _asbp_base_playable) "NewEnumerator4") (Variables|/Game/SpyroContent/Global_Assets/Global_Components/Damageable_Com.Damageable_Com_C|GetHit%20Points (Variables|/Game/SpyroContent/Global_Assets/Global_Characters/Playable_Characters/BP_Base_Playable.BP_Base_Playable_C|GetDamageable _asbp_base_playable)) (select (>= (- (Variables|/Game/SpyroContent/Global_Assets/Global_Components/Damageable_Com.Damageable_Com_C|GetHit%20Points (Variables|/Game/SpyroContent/Global_Assets/Global_Characters/Playable_Characters/BP_Base_Playable.BP_Base_Playable_C|GetDamageable _asbp_base_playable)) 1) 0) (- (Variables|/Game/SpyroContent/Global_Assets/Global_Components/Damageable_Com.Damageable_Com_C|GetHit%20Points (Variables|/Game/SpyroContent/Global_Assets/Global_Characters/Playable_Characters/BP_Base_Playable.BP_Base_Playable_C|GetDamageable _asbp_base_playable)) 1) 0))))
          (if (<= _output_get 0)
            (Default|KillPlayer _asbp_base_playable "NewEnumerator12"))
          (CallFunction|UpdateSkillLevel (* (Variables|Default|GetSkill%20Penalty) -1.0) self))))))