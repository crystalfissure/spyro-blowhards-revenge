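; Short-lived water ripple effect actor for swimmable water that expands and fades out, then destroys itself.
; On BeginPlay it picks a random horizontal target scale, halved when Small is set, and creates a dynamic material instance on its plane.
; Two timelines run in parallel, one lerping actor scale toward the target and one fading the Opacity parameter to zero, before a timed destroy.
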(event Custom|Lerp%20Scale
  (bind _target_scale (Variables|Default|Gettarget%20scale))
  (bind _newtrack_0 (Timeline|Timeline_0 PlayFromStart)
    (:Update
      (Transformation|SetActorScale3D (Math|Vector|Lerp(Vector) (Transformation|GetActorScale3D) (Math|Vector|MakeVector _target_scale _target_scale 1.0) _newtrack_0)))))

(event Custom|Lerp%20Opacity
  (bind _newtrack_0 (Timeline|Timeline_1 PlayFromStart)
    (:Update
      (Rendering|Material|SetScalarParameterValue (Variables|Default|GetRipple_Mat) "Opacity" (Math|Float|Lerp 0.5 0.0 _newtrack_0) :!class /Script/Engine.MaterialInstanceDynamic))))

(event EventBeginPlay
  (bind _returnvalue (Math|Random|RandomFloatinRange 0.4 1.0))
  (bind _plane (Variables|Default|GetPlane))
  (Variables|Default|Settarget%20scale (select (Variables|Default|Getsmall) (* _returnvalue 0.5) _returnvalue))
  (bind _returnvalue_2 (Rendering|Material|CreateDynamicMaterialInstance _plane 0 (Rendering|Material|GetMaterial _plane 0) "None" :!class /Script/Engine.PrimitiveComponent))
  (Variables|Default|SetRipple_Mat _returnvalue_2)
  (CallFunction|LerpOpacity)
  (CallFunction|LerpScale)
  (Utilities|FlowControl|Delay 1.5)
  (Actor|DestroyActor))

(fn ConstructionScript)