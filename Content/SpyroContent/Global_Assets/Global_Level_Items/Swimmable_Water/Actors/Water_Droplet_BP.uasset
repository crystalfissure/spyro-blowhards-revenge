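; Short-lived water droplet actor for swimmable water effects, with a randomized yaw, scale and one of three particle looks.
; Some instances self-destruct on spawn; the rest expire after a delay.
; Tick sweeps it forward at random speeds, boosted by FlyFarther, while a Gravity timeline drives vertical motion.
; Box overlap destroys it on swimmable water or static meshes, spawning a small ripple when it hits the water mesh.
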(event OnComponentBeginOverlap(Box)
  (params (OverlappedComponent :type Primitive%20Component%20Object%20Reference) (OtherActor :type Actor%20Object%20Reference) (OtherComp :type Primitive%20Component%20Object%20Reference) (OtherBodyIndex :type Integer) (bFromSweep :type Boolean) (SweepResult :type Hit%20Result%20Structure%20%28by%20ref%29))
  (bind _returnvalue (Math|Random|RandomFloatinRange 0.1 0.15))
  (bind _returnvalue_2 (Transformation|GetActorTransform))
  (bind _asswimmable_water_bp (Utilities|Casting|CastToSwimmable_Water_BP OtherActor)
    (:then
      (if (== (Variables|/Game/SpyroContent/Global_Assets/Global_Level_Items/Swimmable_Water/Actors/Swimmable_Water_BP.Swimmable_Water_BP_C|GetWater_Mesh _asswimmable_water_bp) OtherComp)
        (Game|SpawnActorfromClass "/Game/SpyroContent/Global_Assets/Global_Level_Items/Swimmable_Water/Actors/Water_Ripple_Small_BP.Water_Ripple_Small_BP_C" (Math|Transform|MakeTransform (.location _returnvalue_2) (Math|Rotator|MakeRotator 0.0 0.0 (.yaw (.rotation _returnvalue_2))) (Math|Vector|MakeVector _returnvalue _returnvalue 1.0)) "AlwaysSpawn" 0 0))
      (Actor|DestroyActor :!label _label))
    (:CastFailed
      (if (== OtherComp (Actor|GetComponentbyClass OtherActor "/Script/Engine.StaticMeshComponent"))
        (goto _label)))))

(event Custom|Gravity
  (bind _newtrack_0 (Timeline|Timeline_0 PlayFromStart)
    (:Update
      (Transformation|AddActorWorldOffset (* (Transformation|GetActorUpVector) (* _newtrack_0 (Math|Random|RandomFloatinRange 1e+01 2e+02) (Utilities|Time|GetWorldDeltaSeconds))) true))))

(event EventBeginPlay
  (bind _returnvalue (Math|Random|RandomFloatinRange 0.2 0.3))
  (if (<= (Math|Random|RandomIntegerinRange 0 7) 0)
    (Actor|DestroyActor)
    (else
      (Transformation|SetActorRotation (Math|Rotator|MakeRotator 0.0 0.0 (+ (.yaw (Transformation|GetActorRotation)) (Math|Random|RandomFloatinRange -3e+01 3e+01))))
      (Transformation|SetActorScale3D (Math|Vector|MakeVector _returnvalue _returnvalue 1.0))
      (Effects|Components|ParticleSystem|SetTemplate (Variables|Default|GetParticleSystem) (Utilities|Select :Index (Math|Random|RandomIntegerinRange 0 2) :Option%200 "/Game/SpyroContent/Global_Assets/Global_Level_Items/Swimmable_Water/Particles/Water_Droplet_Particle.Water_Droplet_Particle" :Option%201 "/Game/SpyroContent/Global_Assets/Global_Level_Items/Swimmable_Water/Particles/Water_Droplet_Particle_Fat.Water_Droplet_Particle_Fat" :Option%202 "/Game/SpyroContent/Global_Assets/Global_Level_Items/Swimmable_Water/Particles/Water_Droplet_Particle_Thin.Water_Droplet_Particle_Thin"))
      (Components|Activation|Activate (Variables|Default|GetParticleSystem) false)
      (CallFunction|Gravity)
      (Utilities|FlowControl|Delay 7.0)
      (Actor|DestroyActor))))

(event EventTick
  (params (DeltaSeconds :type Float%20%28single-precision%29))
  (bind _returnvalue (Math|Random|RandomFloatinRange 1e+01 2.5e+02))
  (Transformation|AddActorWorldOffset (* (Transformation|GetActorForwardVector) (* (Utilities|Time|GetWorldDeltaSeconds) (select (Variables|Default|Getfly%20farther) (* _returnvalue 4.0) _returnvalue))) true))

(fn ConstructionScript)