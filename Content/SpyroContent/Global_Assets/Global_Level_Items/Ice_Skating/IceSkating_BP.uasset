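; Ice skating surface actor that switches overlapping playable characters into an ice ground state.
; Its hitbox copies the ice mesh at BeginPlay; on capsule overlap, a downward trace rules out swimmable water before setting the state, rechecked after a short delay that also stops jumping.
; On exit, a trace slightly ahead of the character keeps the state over other ice actors, otherwise choosing a ground state from the environmental state.
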(event OnComponentBeginOverlap(Ice_Hitbox)
  (params (OverlappedComponent :type Primitive%20Component%20Object%20Reference) (OtherActor :type Actor%20Object%20Reference) (OtherComp :type Primitive%20Component%20Object%20Reference) (OtherBodyIndex :type Integer) (bFromSweep :type Boolean) (SweepResult :type Hit%20Result%20Structure%20%28by%20ref%29))
  (bind _asbp_base_playable (Utilities|Casting|CastToBP_Base_Playable OtherActor))
  (if (Math|Boolean|ANDBoolean (not (Utilities|Enum|Equal(Enum) (Variables|/Game/SpyroContent/Global_Assets/Global_Characters/Playable_Characters/BP_Base_Playable.BP_Base_Playable_C|GetGround_State _asbp_base_playable) "NewEnumerator1")) (not (Utilities|Enum|Equal(Enum) (Variables|/Game/SpyroContent/Global_Assets/Global_Characters/Playable_Characters/BP_Base_Playable.BP_Base_Playable_C|GetEnvironmental_State _asbp_base_playable) "NewEnumerator1")) (== (Variables|/Script/Engine.Character|GetCapsuleComponent _asbp_base_playable) OtherComp))
    (bind _outhit (Collision|LineTraceForObjects (Transformation|GetActorLocation _asbp_base_playable) (Math|Vector|MakeVector (.X (Math|Vector|BreakVector (Transformation|GetActorLocation _asbp_base_playable))) (.Y (Math|Vector|BreakVector (Transformation|GetActorLocation _asbp_base_playable))) (- (.Z (Math|Vector|BreakVector (Transformation|GetActorLocation _asbp_base_playable))) 5e+01)) (Utilities|Array|MakeArray "ObjectTypeQuery1" "ObjectTypeQuery7") false 0 "None"))
    (if (.bblockinghit _outhit)
      (Utilities|Casting|CastToSwimmable_Water_BP (.hitactor _outhit)
        (:CastFailed
          _)))
    (if (Utilities|Enum|Equal(Enum) (Variables|/Game/SpyroContent/Global_Assets/Global_Characters/Playable_Characters/BP_Base_Playable.BP_Base_Playable_C|GetPlayer_State _asbp_base_playable) "NewEnumerator4")
      (Variables|/Game/SpyroContent/Global_Assets/Global_Characters/Playable_Characters/BP_Base_Playable.BP_Base_Playable_C|SetPlayer_State _asbp_base_playable "NewEnumerator0")
      (Variables|/Game/SpyroContent/Global_Assets/Global_Characters/Playable_Characters/BP_Base_Playable.BP_Base_Playable_C|SetGround_State _asbp_base_playable "NewEnumerator2"))
    (Utilities|FlowControl|Delay 0.1)
    (Utilities|IsValid _asbp_base_playable
      (:Is%20Valid
        (Character|StopJumping _asbp_base_playable)
        (if (Math|Boolean|ANDBoolean (Utilities|Enum|Equal(Enum) (Variables|/Game/SpyroContent/Global_Assets/Global_Characters/Playable_Characters/BP_Base_Playable.BP_Base_Playable_C|GetEnvironmental_State _asbp_base_playable) "NewEnumerator0") (not (AI|Components|NavMovement|IsFalling (Variables|/Script/Engine.Character|GetCharacterMovement _asbp_base_playable))) (== OtherComp (Variables|/Script/Engine.Character|GetCapsuleComponent _asbp_base_playable)))
          (Variables|/Game/SpyroContent/Global_Assets/Global_Characters/Playable_Characters/BP_Base_Playable.BP_Base_Playable_C|SetGround_State _asbp_base_playable "NewEnumerator2")
          (if (Utilities|Enum|Equal(Enum) (Variables|/Game/SpyroContent/Global_Assets/Global_Characters/Playable_Characters/BP_Base_Playable.BP_Base_Playable_C|GetPlayer_State _asbp_base_playable) "NewEnumerator4")
            (Variables|/Game/SpyroContent/Global_Assets/Global_Characters/Playable_Characters/BP_Base_Playable.BP_Base_Playable_C|SetPlayer_State _asbp_base_playable "NewEnumerator0")))))))

(event OnComponentEndOverlap(Ice_Hitbox)
  (params (OverlappedComponent :type Primitive%20Component%20Object%20Reference) (OtherActor :type Actor%20Object%20Reference) (OtherComp :type Primitive%20Component%20Object%20Reference) (OtherBodyIndex :type Integer))
  (bind _asbp_base_playable (Utilities|Casting|CastToBP_Base_Playable OtherActor))
  (if (and (== (Variables|/Script/Engine.Character|GetCapsuleComponent _asbp_base_playable) OtherComp) (Utilities|Enum|Equal(Enum) (Variables|/Game/SpyroContent/Global_Assets/Global_Characters/Playable_Characters/BP_Base_Playable.BP_Base_Playable_C|GetGround_State _asbp_base_playable) "NewEnumerator2"))
    (bind _outhit (Collision|LineTraceForObjects (+ (Transformation|GetActorLocation _asbp_base_playable) (* (Transformation|GetActorForwardVector _asbp_base_playable) 2e+01)) (Math|Vector|MakeVector (.X (Math|Vector|BreakVector (+ (Transformation|GetActorLocation _asbp_base_playable) (* (Transformation|GetActorForwardVector _asbp_base_playable) 2e+01)))) (.Y (Math|Vector|BreakVector (+ (Transformation|GetActorLocation _asbp_base_playable) (* (Transformation|GetActorForwardVector _asbp_base_playable) 2e+01)))) (- (.Z (Math|Vector|BreakVector (+ (Transformation|GetActorLocation _asbp_base_playable) (* (Transformation|GetActorForwardVector _asbp_base_playable) 2e+01)))) 75.0)) (Utilities|Array|MakeArray "ObjectTypeQuery1") false 0 "None" false))
    (if (.bblockinghit _outhit)
      (Utilities|Casting|CastToIceSkating_BP (.hitactor _outhit)
        (:CastFailed
          _)))
    (Variables|/Game/SpyroContent/Global_Assets/Global_Characters/Playable_Characters/BP_Base_Playable.BP_Base_Playable_C|SetGround_State _asbp_base_playable (select (Utilities|Enum|Equal(Enum) (Variables|/Game/SpyroContent/Global_Assets/Global_Characters/Playable_Characters/BP_Base_Playable.BP_Base_Playable_C|GetEnvironmental_State _asbp_base_playable) "NewEnumerator0") "NewEnumerator0" "NewEnumerator4"))))

(event EventBeginPlay
  (Components|StaticMesh|SetStaticMesh (Variables|Default|GetIce_Hitbox) (Variables|/Script/Engine.StaticMeshComponent|GetStaticMesh (Variables|Default|GetIce_Mesh))))

(fn ConstructionScript)