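; IceHex_BP is a short-lived ice hex actor for the ice skating level items in the Spyro content.
; On BeginPlay it registers its hitbox with a damageable component and binds a damage event.
; It destroys itself when damaged or after a five-second delay, whichever comes first.
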(event Custom|ice%20hex%20damaged
  (Actor|DestroyActor))

(event EventBeginPlay
  (|CallParentFunction)
  (Variables|/Game/SpyroContent/Global_Assets/Global_Components/Damageable_Com.Damageable_Com_C|SetObject's%20Hitbox%20Component (Variables|Default|GetDamageable_Com) (Variables|Default|Gethitbox))
  (EventDispatchers|BindEventtoCallDealDamage (Variables|Default|GetDamageable_Com) (delegate Custom|ice%20hex%20damaged))
  (Utilities|FlowControl|Delay 5.0)
  (Actor|DestroyActor))

(fn ConstructionScript
  (|CallParentFunction))