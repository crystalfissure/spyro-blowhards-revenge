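; BP_KillPlane is a level kill volume that handles players, gems and spittable objects entering its box.
; A player's capsule overlap kills them and fires APlayerFellInMe, or teleports Spyro to a speedway if flagged, except during black portal transitions.
; Gems are magnetized to the player, or collected when no playable player is found, and spittable objects reset.
; An optional debug flag spawns a tall cylinder where gems touched, exposing gems misplaced under the map.
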(event OnComponentBeginOverlap(Box)
  (params (OverlappedComponent :type Primitive%20Component%20Object%20Reference) (OtherActor :type Actor%20Object%20Reference) (OtherComp :type Primitive%20Component%20Object%20Reference) (OtherBodyIndex :type Integer) (bFromSweep :type Boolean) (SweepResult :type Hit%20Result%20Structure%20%28by%20ref%29))
  (bind _asbp_base_playable (Utilities|Casting|CastToBP_Base_Playable OtherActor)
    (:then
      (if (and (== (Variables|/Script/Engine.Character|GetCapsuleComponent _asbp_base_playable) OtherComp) (not (Variables|/Game/SpyroContent/Global_Assets/Global_Characters/Playable_Characters/BP_Base_Playable.BP_Base_Playable_C|GetIn_BlackPortal_Transition _asbp_base_playable)))
        ;[0.207 0.03193 0.5573] qtderg experimental modification
        ;
        ; Teleporting to a speedway start
        (if (Variables|Default|GetTeleportsToASpeedway)
          (bind _asbp_spyro (Utilities|Casting|CastToBP_Spyro _asbp_base_playable))
          (Default|TeleporttoSpeedway _asbp_spyro)
          (else
            (Default|KillPlayer _asbp_base_playable "NewEnumerator5")
            (Default|CallAPlayerFellinMe)))))
    (:CastFailed
      (bind _asgem_base_bp (Utilities|Casting|CastToGem_Base_BP OtherActor)
        (:then
          (Utilities|IsValid _asgem_base_bp
            (:Is%20Valid
              (if (not (Utilities|Enum|Equal(Enum) (Variables|/Game/SpyroContent/Global_Assets/Global_Level_Items/Gems/Actors/Gem_Base_BP.Gem_Base_BP_C|GetGem_State _asgem_base_bp) "NewEnumerator2"))
                (bind _asbp_base_playable_2 (Utilities|Casting|CastToBP_Base_Playable (Game|GetPlayerCharacter 0))
                  (:then
                    (Default|ChangeGemState _asgem_base_bp "NewEnumerator3" _asbp_base_playable_2))
                  (:CastFailed
                    (Default|CollectGem _asgem_base_bp)))
                (Development|PrintString "BPKillPnae: A GEM TOUCHED THE KILL PLANE")
                ;[0.207 0.03193 0.5573] qtderg contribution
                ;
                ; Gem touch visualizer, helpful when you accidentally place a gem under the map
                (if (Variables|Default|GetDEBUG%20Spawn%20gem%20touch%20visualizer)
                  (bind _returnvalue (Game|SpawnActorfromClass "/Script/Engine.StaticMeshActor" (Math|Transform|MakeTransform (Transformation|GetActorLocation _asgem_base_bp) "0, 0, 0" "0.250000,0.250000,250.000000") "Undefined" 0 0))
                  (Transformation|SetMobility _returnvalue "Movable")
                  (Components|StaticMesh|SetStaticMesh (Variables|/Script/Engine.StaticMeshActor|GetStaticMeshComponent _returnvalue) "/Engine/BasicShapes/Cylinder.Cylinder")
                  (Rendering|Material|SetMaterial (Variables|/Script/Engine.StaticMeshActor|GetStaticMeshComponent _returnvalue) 0 "/Game/SpyroContent/Global_Assets/Global_Materials/Material_Instances/Untex_Vertex_Color_2Sided.Untex_Vertex_Color_2Sided"))))))
        (:CastFailed
          (bind _asbase_spittable_object_bp (Utilities|Casting|CastToBase_Spittable_Object_BP OtherActor))
          (Default|ResetSpittableObject _asbase_spittable_object_bp))))))

(event EventBeginPlay)

(event Collision|EventActorBeginOverlap
  (params (OtherActor :type Actor%20Object%20Reference)))

(event EventTick
  (params (DeltaSeconds :type Float%20%28single-precision%29)))

(fn ConstructionScript)