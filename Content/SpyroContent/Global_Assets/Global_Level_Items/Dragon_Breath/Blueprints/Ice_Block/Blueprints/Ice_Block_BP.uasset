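; Ice block actor that encases a character frozen by ice breath, or stands empty, until it melts or is shattered.
; A one-second looping timer counts down to Melt, which fades the dynamic material, plays a melt animation and releases the character.
; Its Damageable component routes hits: Freeze resets the countdown and normal Burn melts it.
; Other hits spawn a destructible block, thaw the captive and usually forward the damage.
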(event Custom|Ice%20Damage%20Procedure
  (params (Attacker's%20Forward%20Vector :type Vector) (Damage%20Type :type Damage_Types%20Enum :default "NewEnumerator6") (Delay :type Float%20%28single-precision%29) (Super? :type Boolean))
  (bind _frozen_character (Variables|Default|GetFrozen_Character))
  (bind _frozen_character_2 (Variables|Default|GetFrozen_Character))
  (bind _ice_block (Variables|Default|GetIce_Block))
  (bind _returnvalue (Actor|GetComponentbyClass _frozen_character_2 "/Game/SpyroContent/Global_Assets/Global_Components/Damageable_Com.Damageable_Com_C"))
  (bind _frozen_character_3 (Variables|Default|GetFrozen_Character)
    (:then
      (Game|SpawnActorfromClass "/Game/SpyroContent/Global_Assets/Global_Level_Items/Dragon_Breath/Blueprints/Ice_Block/Blueprints/Ice_Block_Destructable_BP.Ice_Block_Destructable_BP_C" (Transformation|GetActorTransform) "AlwaysSpawn" 0 0)
      (Physics|SetSimulatePhysics _ice_block false)
      (Collision|SetCollisionEnabled _ice_block "NoCollision")
      (if (Variables|/Game/SpyroContent/Global_Assets/Global_Components/Damageable_Com.Damageable_Com_C|GetInvincible _returnvalue)
        (bind _asbase_enemy_bp (Utilities|Casting|CastToBase_Enemy_BP (Variables|Default|GetFrozen_Character))
          (:then
            (if (Variables|/Game/SpyroContent/Global_Assets/Global_Characters/AI_Characters/Actors/Enemies/Base_Enemy_BP.Base_Enemy_BP_C|Getcan%20freeze%20but%20cant%20die _asbase_enemy_bp)
              (Default|MeltWithoutDisablingInvincibility (Variables|/Game/SpyroContent/Global_Assets/Global_Characters/AI_Characters/Actors/Base_AICharacter_BP.Base_AICharacter_BP_C|GetDamageable _asbase_enemy_bp)))
            (Actor|DestroyActor))
          (:CastFailed
            (Variables|/Game/SpyroContent/Global_Assets/Global_Components/Damageable_Com.Damageable_Com_C|SetDamage_Being_Taken (Actor|GetComponentbyClass _frozen_character_3 "/Game/SpyroContent/Global_Assets/Global_Components/Damageable_Com.Damageable_Com_C") "NewEnumerator6" :!label _label)
            (Utilities|Casting|CastToBase_Enemy_BP _frozen_character
              (:then
                (Variables|/Script/Engine.Actor|SetCustomTimeDilation _frozen_character_3 1.0 :!label _label_2)
                (Variables|/Game/SpyroContent/Global_Assets/Global_Components/Damageable_Com.Damageable_Com_C|SetFrozen (Actor|GetComponentbyClass _frozen_character_3 "/Game/SpyroContent/Global_Assets/Global_Components/Damageable_Com.Damageable_Com_C") false))
              (:CastFailed
                (bind _asbp_base_playable (Utilities|Casting|CastToBP_Base_Playable _frozen_character)
                  (:then
                    (Collision|SetCollisionObjectType (Variables|/Script/Engine.Character|GetCapsuleComponent _asbp_base_playable) "ECC_Pawn")
                    (goto _label_2))
                  (:CastFailed
                    (bind _asnpc_base_bp (Utilities|Casting|CastToNPC_Base_BP _frozen_character)
                      (:then
                        (Collision|SetCollisionObjectType (Variables|/Script/Engine.Character|GetCapsuleComponent _asnpc_base_bp) "ECC_Pawn")
                        (if (Math|Boolean|ANDBoolean (Utilities|Enum|Equal(Enum) (Variables|/Game/SpyroContent/Global_Assets/Global_Characters/NPCs/NPC_Base_BP.NPC_Base_BP_C|GetNPC_State _asnpc_base_bp) "NewEnumerator3") (Utilities|Enum|Equal(Enum) (Variables|/Game/SpyroContent/Global_Assets/Global_Components/Damageable_Com.Damageable_Com_C|GetDamage_Being_Taken (Variables|/Game/SpyroContent/Global_Assets/Global_Characters/NPCs/NPC_Base_BP.NPC_Base_BP_C|GetNPC_Damageable _asnpc_base_bp)) "NewEnumerator6") (Variables|/Game/SpyroContent/Global_Assets/Global_Components/Damageable_Com.Damageable_Com_C|GetFrozen (Variables|/Game/SpyroContent/Global_Assets/Global_Characters/NPCs/NPC_Base_BP.NPC_Base_BP_C|GetNPC_Damageable _asnpc_base_bp)))
                          (goto _label_2)
                          (else
                            _)))
                      (:CastFailed
                        _))))))
            (Default|MeltWithoutDisablingInvincibility _returnvalue)
            (bind _asbase_enemy_bp_2 (Utilities|Casting|CastToBase_Enemy_BP _frozen_character_2)
              (:then
                (Default|ForceDamageReset (Variables|/Game/SpyroContent/Global_Assets/Global_Characters/AI_Characters/Actors/Base_AICharacter_BP.Base_AICharacter_BP_C|GetWalking_AI_Character _asbase_enemy_bp_2)))
              (:CastFailed
                _))
            (Default|DealDamage _returnvalue Damage%20Type Attacker's%20Forward%20Vector (select (or (Utilities|Enum|Equal(Enum) Damage%20Type "NewEnumerator4") Super?) true false) 0 false)
            (Development|PrintString "IceBlockBP: HURT WHILE IN ICE, TAKE DAMAGE" true true "(R=0.000000,G=0.660000,B=1.000000,A=1.000000)" 3e+01)
            (Utilities|FlowControl|Delay Delay)
            (Actor|DestroyActor)))
        (else
          (goto _label))))
    (:else
      (if (Variables|Default|Getno%20frozen%20character)
        (Game|SpawnActorfromClass "/Game/SpyroContent/Global_Assets/Global_Level_Items/Dragon_Breath/Blueprints/Ice_Block/Blueprints/Ice_Block_Destructable_BP.Ice_Block_Destructable_BP_C" (Transformation|GetActorTransform) "AlwaysSpawn" 0 0)
        (Actor|DestroyActor)
        (else
          (Development|PrintString "CANNOT DESTROY ICE, FROZEN CHARACTER IS INVALID"))))))

(event Custom|Melt
  (Utilities|FlowControl|DoOnce false
    (:Completed
      (bind _frozen_character (Variables|Default|GetFrozen_Character)
        (:then
          (bind _asbase_enemy_bp (Utilities|Casting|CastToBase_Enemy_BP _frozen_character)
            (:then
              (Variables|/Game/SpyroContent/Global_Assets/Global_Components/Damageable_Com.Damageable_Com_C|SetInvincible (Variables|/Game/SpyroContent/Global_Assets/Global_Characters/AI_Characters/Actors/Base_AICharacter_BP.Base_AICharacter_BP_C|GetDamageable _asbase_enemy_bp) true))
            (:CastFailed
              (bind _asnpc_base_bp (Utilities|Casting|CastToNPC_Base_BP _frozen_character)
                (:then
                  (Variables|/Game/SpyroContent/Global_Assets/Global_Components/Damageable_Com.Damageable_Com_C|SetInvincible (Variables|/Game/SpyroContent/Global_Assets/Global_Characters/NPCs/NPC_Base_BP.NPC_Base_BP_C|GetNPC_Damageable _asnpc_base_bp) true))
                (:CastFailed
                  _)))))
        (:else
          _))
      (Components|Animation|PlayAnimation (Variables|Default|GetSkeletalMesh) "/Game/SpyroContent/Global_Assets/Global_Level_Items/Dragon_Breath/Blueprints/Ice_Block/Animations/ice_block_skeletal_Anim_Armature_Melting.ice_block_skeletal_Anim_Armature_Melting" false)
      (Physics|SetSimulatePhysics (Variables|Default|GetIce_Block) false)
      (Collision|SetCollisionEnabled (Variables|Default|GetIce_Block) "NoCollision")
      (bind _newtrack_0 (Timeline|Timeline_0 PlayFromStart)
        (:Update
          (Rendering|Material|SetScalarParameterValue (Variables|Default|GetMat_Instance) "Opacity" (Math|Float|Lerp 0.5 0.0 _newtrack_0) :!class /Script/Engine.MaterialInstanceDynamic))
        (:Finished
          (bind _frozen_character_2 (Variables|Default|GetFrozen_Character)
            (:then
              (Default|Melt (Actor|GetComponentbyClass _frozen_character_2 "/Game/SpyroContent/Global_Assets/Global_Components/Damageable_Com.Damageable_Com_C")))
            (:else
              _))
          (Actor|DestroyActor))))))

(event Custom|Deal%20Damage%20to%20Ice%20Block
  (bind _damageable (Variables|Default|GetDamageable))
  (bind _deal_damage___super_damage (Variables|/Game/SpyroContent/Global_Assets/Global_Components/Damageable_Com.Damageable_Com_C|GetDeal%20Damage%20-%20Super%20Damage _damageable))
  (switch Utilities|FlowControl|Switch|SwitchonDamage_Types (Variables|/Game/SpyroContent/Global_Assets/Global_Components/Damageable_Com.Damageable_Com_C|GetDeal%20Damage%20-%20Damage%20Type (Variables|Default|GetDamageable))
    (:NewEnumerator0
      (CallFunction|IceDamageProcedure "0, 0, 0" "NewEnumerator0" 0.0 _deal_damage___super_damage))
    (:NewEnumerator1
      (if _deal_damage___super_damage
        (CallFunction|IceDamageProcedure "0, 0, 0" "NewEnumerator1" 0.0 true)
        (else
          (CallFunction|Melt))))
    (:NewEnumerator2
      (CallFunction|IceDamageProcedure "0, 0, 0" "NewEnumerator2" 0.0 _deal_damage___super_damage))
    (:NewEnumerator3
      (CallFunction|IceDamageProcedure "0, 0, 0" "NewEnumerator3" 0.0 _deal_damage___super_damage))
    (:NewEnumerator4
      (CallFunction|IceDamageProcedure (Variables|/Game/SpyroContent/Global_Assets/Global_Components/Damageable_Com.Damageable_Com_C|GetDeal%20Damage%20-%20Attackers%20Forward%20Vector (Variables|Default|GetDamageable)) "NewEnumerator4" 0.1 _deal_damage___super_damage))
    (:NewEnumerator7
      (Variables|Default|SetMeltdown_Time (Variables|Default|GetDefault%20Meltdown%20Time)))))

(event EventBeginPlay
  (bind _skeletalmesh (Variables|Default|GetSkeletalMesh))
  (bind _damageable (Variables|Default|GetDamageable))
  (Audio|PlaySoundatLocation "/Game/SpyroContent/Global_Assets/Global_Level_Items/Dragon_Breath/Blueprints/Ice_Block/Audio/ice_impact.ice_impact" (Transformation|GetActorLocation) "0, 0, 0" 1.0 1.0 0.0 0 0 0)
  (bind _returnvalue (Rendering|Material|CreateDynamicMaterialInstance _skeletalmesh 0 (Rendering|Material|GetMaterial _skeletalmesh 0) "None" :!class /Script/Engine.PrimitiveComponent))
  (Variables|Default|SetMat_Instance _returnvalue)
  (Utilities|Time|SetTimerbyFunctionName 0 "Melt Countdown" 1.0 true)
  (EventDispatchers|BindEventtoCallDealDamage _damageable (delegate Custom|Deal%20Damage%20to%20Ice%20Block))
  (Variables|/Game/SpyroContent/Global_Assets/Global_Components/Damageable_Com.Damageable_Com_C|SetObject's%20Hitbox%20Component _damageable (Variables|Default|GetIce_Block)))

(fn ConstructionScript)

(fn MeltCountdown
  (if (> (Variables|Default|GetMeltdown_Time) 0)
    (Variables|Default|SetMeltdown_Time (- (Variables|Default|GetMeltdown_Time) 1))
    (bind _frozen_character (Variables|Default|GetFrozen_Character)
      (:then
        (Utilities|IsValid (Actor|GetComponentbyClass _frozen_character "/Game/SpyroContent/Global_Assets/Global_Components/Damageable_Com.Damageable_Com_C")
          (:Is%20Valid
            (if (not (Variables|/Game/SpyroContent/Global_Assets/Global_Components/Damageable_Com.Damageable_Com_C|GetFrozen (Actor|GetComponentbyClass _frozen_character "/Game/SpyroContent/Global_Assets/Global_Components/Damageable_Com.Damageable_Com_C")))
              (CallFunction|Melt)))))
      (:else))
    (else
      (CallFunction|Melt))))