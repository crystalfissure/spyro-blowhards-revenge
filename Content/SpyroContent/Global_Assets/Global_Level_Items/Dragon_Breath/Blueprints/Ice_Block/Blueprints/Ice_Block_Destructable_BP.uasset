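; Destructible ice block actor that plays a one-shot shatter effect as soon as it begins play.
; BeginPlay plays the shatter sound and applies radius damage with an impulse at the Destructible component's location to break it apart.
; A timeline then fades the Opacity parameter on a dynamic material instance from semi-transparent to invisible, and the actor destroys itself when the fade finishes.
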(event EventBeginPlay
  (bind _destructible (Variables|Default|GetDestructible))
  (bind _destructible_2 (Variables|Default|GetDestructible))
  (Audio|PlaySoundatLocation "/Game/SpyroContent/Global_Assets/Global_Level_Items/Dragon_Breath/Blueprints/Ice_Block/Audio/ice_shatter.ice_shatter" (Transformation|GetActorLocation) "0, 0, 0" 1.0 1.0 0.0 0 0 0)
  (Class|DestructibleComponent|ApplyRadiusDamage _destructible 2e+01 (Transformation|GetWorldLocation _destructible) 6e+01 5e+03 false)
  (bind _returnvalue (Rendering|Material|CreateDynamicMaterialInstance _destructible_2 0 (Rendering|Material|GetMaterial _destructible_2 0) "None" :!class /Script/Engine.PrimitiveComponent))
  (Variables|Default|SetMat%20Instance _returnvalue)
  (bind _newtrack_0 (Timeline|Timeline_0 PlayFromStart)
    (:Update
      (Rendering|Material|SetScalarParameterValue (Variables|Default|GetMat%20Instance) "Opacity" (Math|Float|Lerp 0.5 0.0 _newtrack_0) :!class /Script/Engine.MaterialInstanceDynamic))
    (:Finished
      (Actor|DestroyActor))))

(fn ConstructionScript)