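; Fear_Manager is a Blueprint in the Dragon Breath items that pulls its owning character downward, apparently while that character is under a fear effect.
; Each tick, if the character's capsule has gravity enabled, it moves the character down at a constant speed with a swept SetActorLocation.
; Characters whose Damageable_Com flags them to float when frozen or feared are skipped, while those lacking that component still descend.
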(event EventTick
  (params (DeltaSeconds :type Float%20%28single-precision%29))
  (bind _owning_character (Variables|Default|GetOwning_Character)
    (:then
      (if (Class|PrimitiveComponent|IsGravityEnabled (Variables|/Script/Engine.Character|GetCapsuleComponent _owning_character))
        (bind _asdamageable_co (Utilities|Casting|CastToDamageable_Com (Actor|GetComponentbyClass _owning_character "/Game/SpyroContent/Global_Assets/Global_Components/Damageable_Com.Damageable_Com_C"))
          (:then
            (if (not (Variables|/Game/SpyroContent/Global_Assets/Global_Components/Damageable_Com.Damageable_Com_C|GetFloats%20when%20frozen%20in%20ice%20or%20fear _asdamageable_co))
              (Transformation|SetActorLocation _owning_character (Math|Vector|MakeVector (.x (Transformation|GetActorLocation _owning_character)) (.y (Transformation|GetActorLocation _owning_character)) (+ (.z (Transformation|GetActorLocation _owning_character)) (* DeltaSeconds -3.2e+02))) true false :!label _label)))
          (:CastFailed
            (goto _label)))))
    (:else)))

(fn ConstructionScript)