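; Spawner that periodically spits lava by spawning an actor of a configurable class at its root transform while players are nearby.
; A playable's capsule entering AwakeHitbox triggers an immediate spit and restarts a looping timer at the Frequency interval.
; It tracks players in range and clears the timer when the last one leaves.
; On BeginPlay, a timeline grows AwakeHitbox from a tenth scale to full size.
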(event OnComponentBeginOverlap(AwakeHitbox)
  (params (OverlappedComponent :type Primitive%20Component%20Object%20Reference) (OtherActor :type Actor%20Object%20Reference) (OtherComp :type Primitive%20Component%20Object%20Reference) (OtherBodyIndex :type Integer) (bFromSweep :type Boolean) (SweepResult :type Hit%20Result%20Structure%20%28by%20ref%29))
  (bind _asbp_base_playable (Utilities|Casting|CastToBP_Base_Playable OtherActor))
  (if (== (Variables|/Script/Engine.Character|GetCapsuleComponent _asbp_base_playable) OtherComp)
    (Utilities|Array|AddUnique (Variables|Default|GetPlayers%20in%20My%20Range) _asbp_base_playable)
    (Utilities|Time|ClearandInvalidateTimerbyHandle (Variables|Default|GetTimer))
    (CallFunction|SpitLava)
    (bind _returnvalue (Utilities|Time|SetTimerbyFunctionName 0 "Spit Lava" (Variables|Default|GetFrequency) true))
    (Variables|Default|SetTimer _returnvalue)))

(event OnComponentEndOverlap(AwakeHitbox)
  (params (OverlappedComponent :type Primitive%20Component%20Object%20Reference) (OtherActor :type Actor%20Object%20Reference) (OtherComp :type Primitive%20Component%20Object%20Reference) (OtherBodyIndex :type Integer))
  (bind _asbp_base_playable (Utilities|Casting|CastToBP_Base_Playable OtherActor))
  (if (== (Variables|/Script/Engine.Character|GetCapsuleComponent _asbp_base_playable) OtherComp)
    (Utilities|Array|RemoveItem (Variables|Default|GetPlayers%20in%20My%20Range) _asbp_base_playable)
    (if (<= (Utilities|Array|Length (Variables|Default|GetPlayers%20in%20My%20Range)) 0)
      (Utilities|Time|ClearandInvalidateTimerbyHandle (Variables|Default|GetTimer)))))

(event EventBeginPlay
  (Transformation|SetRelativeScale3D (Variables|Default|GetAwake%20Hitbox) "0.100000,0.100000,0.100000")
  (bind _newtrack_0 (Timeline|Timeline_0 PlayFromStart)
    (:Update
      (Transformation|SetRelativeScale3D (Variables|Default|GetAwake%20Hitbox) (Math|Vector|Lerp(Vector) "0.100000,0.100000,0.100000" "1.000000,1.000000,1.000000" _newtrack_0)))))

(fn ConstructionScript)

(fn SpitLava
  (Game|SpawnActorfromClass (Variables|Default|GetClass) (Transformation|GetWorldTransform (Variables|Default|GetDefaultSceneRoot)) "AlwaysSpawn" 0 0))