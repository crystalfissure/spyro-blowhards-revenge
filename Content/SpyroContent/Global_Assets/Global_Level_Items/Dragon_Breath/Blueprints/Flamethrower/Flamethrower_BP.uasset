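; Flamethrower dragon breath actor that deals super damage through a timed box hitbox, then destroys itself.
; After a start delay it moves and enlarges the box, removes it after an end delay, and lingers briefly before cleanup, longer when NoOwner is set.
; Overlaps damage only a Damageable_Com's designated hitbox, skipping the owner.
; Without a valid owner, damage applies only if NoOwner is set.
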(event OnComponentBeginOverlap(Box)
  (params (OverlappedComponent :type Primitive%20Component%20Object%20Reference) (OtherActor :type Actor%20Object%20Reference) (OtherComp :type Primitive%20Component%20Object%20Reference) (OtherBodyIndex :type Integer) (bFromSweep :type Boolean) (SweepResult :type Hit%20Result%20Structure%20%28by%20ref%29))
  (CallFunction|DamageTarget? OtherActor OtherComp))

(event EventBeginPlay
  (bind _box (Variables|Default|GetBox))
  (Utilities|FlowControl|Delay (Variables|Default|GetStartt%20Delay))
  (Transformation|SetRelativeLocation (Variables|Default|GetBox) "220.000000, 0, 0" false false)
  (Transformation|SetRelativeScale3D _box (* (Variables|/Script/Engine.SceneComponent|GetRelativeScale3D _box) 1e+01))
  (Variables|Default|SetCustomTimeDilation 1.5)
  (Utilities|FlowControl|Delay (Variables|Default|GetEnd%20Delay))
  (Components|DestroyComponent (Variables|Default|GetBox))
  (Utilities|FlowControl|Delay (select (Variables|Default|GetNo%20Owner) 7.0 1.0))
  (Actor|DestroyActor))

(fn ConstructionScript)

(fn DamageTarget?
  (params (Other%20Actor :type Actor%20Object%20Reference) (Other%20Comp :type Actor%20Component%20Object%20Reference))
  (bind _returnvalue (Actor|GetComponentbyClass Other%20Actor "/Game/SpyroContent/Global_Assets/Global_Components/Damageable_Com.Damageable_Com_C"))
  (Utilities|IsValid _returnvalue
    (:Is%20Valid
      (if (== (Variables|/Game/SpyroContent/Global_Assets/Global_Components/Damageable_Com.Damageable_Com_C|GetObject's%20Hitbox%20Component _returnvalue) Other%20Comp)
        (bind _myowner (Variables|Default|GetMyOwner)
          (:then
            (if (not (== _myowner Other%20Actor))
              (Default|DealDamage _returnvalue "NewEnumerator1" "0, 0, 0" true (Variables|Default|GetMyOwner) false)))
          (:else
            (if (Variables|Default|GetNo%20Owner)
              (Default|DealDamage _returnvalue "NewEnumerator1" "0, 0, 0" true 0 false))))))))