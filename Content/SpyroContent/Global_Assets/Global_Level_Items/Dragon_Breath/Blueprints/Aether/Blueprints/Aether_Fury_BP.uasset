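; Aether Fury is a short-lived dragon breath burst that deals super damage to damageable actors it overlaps, excluding its creator.
; On spawn it plays a sound, while timelines scale the mesh and drive its dynamic material's opacity, then destroys itself after a brief delay.
; Sphere overlaps damage through Damageable_Com when hitting its hitbox, with a Character capsule fallback added as a workaround for egg thieves.
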(event OnComponentBeginOverlap(Sphere)
  (params (OverlappedComponent :type Primitive%20Component%20Object%20Reference) (OtherActor :type Actor%20Object%20Reference) (OtherComp :type Primitive%20Component%20Object%20Reference) (OtherBodyIndex :type Integer) (bFromSweep :type Boolean) (SweepResult :type Hit%20Result%20Structure%20%28by%20ref%29))
  (CallFunction|ShouldIDamage? OtherActor OtherComp))

(event EventBeginPlay
  (bind _staticmesh (Variables|Default|GetStaticMesh))
  (Audio|PlaySoundatLocation "/Game/SpyroContent/Global_Assets/Global_Level_Items/Superflame/Audio/underwater_superflame_sound.underwater_superflame_sound" (Transformation|GetActorLocation) "0, 0, 0" 1.0 1.0 0.0 0 0 0)
  (bind _returnvalue (Rendering|Material|CreateDynamicMaterialInstance _staticmesh 0 (Rendering|Material|GetMaterial _staticmesh 0) "None" :!class /Script/Engine.PrimitiveComponent))
  (Variables|Default|SetMat_Inst _returnvalue)
  (Utilities|FlowControl|Sequence
    (:then_0
      (bind _newtrack_0 (Timeline|Timeline_0 PlayFromStart)
        (:Update
          (Transformation|SetRelativeScale3D (Variables|Default|GetStaticMesh) (Math|Vector|MakeVector _newtrack_0 _newtrack_0 _newtrack_0)))))
    (:then_1
      (bind _newtrack_0_2 (Timeline|Timeline_1 PlayFromStart)
        (:Update
          (Rendering|Material|SetScalarParameterValue (Variables|Default|GetMat_Inst) "Opacity" _newtrack_0_2 :!class /Script/Engine.MaterialInstanceDynamic))))
    (:then_2
      (Utilities|FlowControl|Delay 0.7)
      (Actor|DestroyActor))))

(fn ConstructionScript)

(fn ShouldIDamage?
  (params (Other%20Actor :type Actor%20Object%20Reference) (Other%20Component :type Actor%20Component%20Object%20Reference))
  (bind _returnvalue (Actor|GetComponentbyClass Other%20Actor "/Game/SpyroContent/Global_Assets/Global_Components/Damageable_Com.Damageable_Com_C"))
  (Utilities|IsValid Other%20Actor
    (:Is%20Valid
      (Utilities|IsValid _returnvalue
        (:Is%20Valid
          (bind _mycreator (Variables|Default|GetMyCreator)
            (:then
              (if (and (not (== _mycreator Other%20Actor)) (== Other%20Component (Variables|/Game/SpyroContent/Global_Assets/Global_Components/Damageable_Com.Damageable_Com_C|GetObject's%20Hitbox%20Component _returnvalue)))
                (Default|DealDamage _returnvalue "NewEnumerator0" "0, 0, 0" true (Variables|Default|GetMyCreator) true :!label _label)
                (else
                  (bind _ascharacter (Utilities|Casting|CastToCharacter Other%20Actor))
                  (if (and (== (Variables|/Script/Engine.Character|GetCapsuleComponent _ascharacter) Other%20Component) (not (== _mycreator Other%20Actor)))
                    (goto _label)))))
            (:else)))))))