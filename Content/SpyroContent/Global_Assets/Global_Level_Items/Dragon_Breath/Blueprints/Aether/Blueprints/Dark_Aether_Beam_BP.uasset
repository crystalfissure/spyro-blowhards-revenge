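; Dark Aether breath beam actor for Spyro that deals continuous super damage along his line of aim while the flame button is held.
; SpawnLazer attaches a beam emitter at the head, and the actor destroys itself if its creator already has one.
; Tick box-traces from head or camera aim to set beam endpoints, damage Damageable components and trigger throttled blast effects.
; It self-destructs on button release, breath change, disabling states or level transition.
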(event Custom|Spawn%20Lazer
  (Transformation|AttachComponentToComponent (Variables|Default|GetDark_Aether_Spawn_Particle) (Variables|/Script/Engine.Character|GetMesh (Variables|Default|GetMyCreator)) "Head" "KeepWorld" "KeepWorld" "KeepWorld" true)
  (bind _returnvalue (Effects|SpawnEmitterAttached "/Game/SpyroContent/Global_Assets/Global_Level_Items/Dragon_Breath/Blueprints/Aether/Particles/Dark_Aether_Beam_Particle.Dark_Aether_Beam_Particle" (Variables|/Script/Engine.Character|GetMesh (Variables|Default|GetMyCreator)) "Head"))
  (Variables|/Script/Engine.ParticleSystemComponent|SetCustomTimeDilation _returnvalue 8.0)
  (Variables|Default|SetLazer_Ref _returnvalue)
  (bind _outactors (Actor|GetAllActorsOfClass "Dark_Aether_Beam_BP_C"))
  (for _array_element _outactors
    (Utilities|IsValid _array_element
      (:Is%20Valid
        (if (and (== (Variables|Dark_Aether_Beam_BP_C|GetMyCreator _array_element) (Variables|Default|GetMyCreator)) (not (== _array_element self)))
          (Actor|DestroyActor))))))

(event Custom|Self%20Destruct
  (Actor|DestroyActor))

(event Custom|Unlock%20Explosion
  (Utilities|FlowControl|DoOnce false) ; enters at Reset
)

(event EventTick
  (params (DeltaSeconds :type Float%20%28single-precision%29))
  (bind (_returnvalue _returnvalue2) (|Spyro'sHead'sForwardVector))
  (bind _mycreator (Variables|Default|GetMyCreator))
  (bind _mycreator_2 (Variables|Default|GetMyCreator))
  (bind _mycreator_3 (Variables|Default|GetMyCreator))
  (bind _mycreator_4 (Variables|Default|GetMyCreator))
  (bind _returnvalue_2 (|StartingPoint _returnvalue))
  (bind _followcamera (Variables|/Game/SpyroContent/Global_Assets/Global_Characters/Playable_Characters/BP_Base_Playable.BP_Base_Playable_C|GetFollowCamera _mycreator))
  (bind _mesh (Variables|/Script/Engine.Character|GetMesh _mycreator_3))
  (bind _player_state (Variables|/Game/SpyroContent/Global_Assets/Global_Characters/Playable_Characters/BP_Base_Playable.BP_Base_Playable_C|GetPlayer_State _mycreator_4))
  (bind _returnvalue_3 (Math|Vector|GetForwardVector _followcamera))
  (bind _returnvalue_4 (Transformation|GetSocketLocation _mesh "Head"))
  (bind _returnvalue_5 (Utilities|Enum|Equal(Enum) _player_state "NewEnumerator14"))
  (bind _returnvalue_6 (select _returnvalue_5 _returnvalue_3 _returnvalue))
  (bind _returnvalue_7 (* _returnvalue_6 1e+04))
  (bind _returnvalue_8 (+ _returnvalue_4 _returnvalue_7))
  (bind _mycreator_5 (Variables|Default|GetMyCreator)
    (:then
      (bind _returnvalue_9 (Default|IsFlameButtonHeldFunction _mycreator_5))
      (if (Math|Boolean|ORBoolean (not _returnvalue_9) (not (Utilities|Enum|Equal(Enum) (Variables|/Game/SpyroContent/Global_Assets/Global_Characters/Playable_Characters/Spyro/BP_Spyro.BP_Spyro_C|GetBreath_Spyro_is_Going_to_Shoot_Next _mycreator_5) "NewEnumerator18")) (Utilities|Enum|Equal(Enum) (Variables|/Game/SpyroContent/Global_Assets/Global_Characters/Playable_Characters/BP_Base_Playable.BP_Base_Playable_C|GetPlayer_State _mycreator_5) "NewEnumerator11") (Utilities|Enum|Equal(Enum) (Variables|/Game/SpyroContent/Global_Assets/Global_Characters/Playable_Characters/BP_Base_Playable.BP_Base_Playable_C|GetPlayer_State _mycreator_5) "NewEnumerator5") (Utilities|Enum|Equal(Enum) (Variables|/Game/SpyroContent/Global_Assets/Global_Characters/Playable_Characters/BP_Base_Playable.BP_Base_Playable_C|GetPlayer_State _mycreator_5) "NewEnumerator8") (Utilities|Enum|Equal(Enum) (Variables|/Game/SpyroContent/Global_Assets/Global_Characters/Playable_Characters/BP_Base_Playable.BP_Base_Playable_C|GetPlayer_State _mycreator_5) "NewEnumerator18") (Variables|/Game/SpyroContent/Global_Assets/Global_Components/Damageable_Com.Damageable_Com_C|GetFrozen (Variables|/Game/SpyroContent/Global_Assets/Global_Characters/Playable_Characters/BP_Base_Playable.BP_Base_Playable_C|GetDamageable _mycreator_5)) (Variables|/Game/SpyroContent/Global_Assets/Global_Components/Damageable_Com.Damageable_Com_C|GetParalyzed_by_Fear (Variables|/Game/SpyroContent/Global_Assets/Global_Characters/Playable_Characters/BP_Base_Playable.BP_Base_Playable_C|GetDamageable _mycreator_5)))
        (Actor|DestroyActor)
        (else
          (Transformation|SetWorldLocationAndRotation (Variables|Default|GetDark_Aether_Spawn_Particle) (select (Utilities|Enum|Equal(Enum) (Variables|/Game/SpyroContent/Global_Assets/Global_Characters/Playable_Characters/BP_Base_Playable.BP_Base_Playable_C|GetPlayer_State (Variables|Default|GetMyCreator)) "NewEnumerator14") "0, 0, 0" (+ (Transformation|GetSocketLocation (Variables|/Script/Engine.Character|GetMesh (Variables|Default|GetMyCreator)) "Head") (* _returnvalue 3e+01))) _returnvalue2 false false)
          (bind _lazer_ref (Variables|Default|GetLazer_Ref)
            (:then
              (Class|ParticleSystemComponent|SetBeamSourcePoint _lazer_ref 0 _returnvalue_2)
              (bind _outhit (Class|KismetSystemLibrary|BoxTraceSingleforObjects _returnvalue_2 _returnvalue_8 "10.000000,10.000000,10.000000" "0, 0, 0" (Utilities|Array|MakeArray "ObjectTypeQuery1" "ObjectTypeQuery3" "ObjectTypeQuery8" "ObjectTypeQuery9" "ObjectTypeQuery10") false (Utilities|Array|MakeArray (Variables|Default|GetMyCreator)) "None" true))
              (Class|ParticleSystemComponent|SetBeamEndPoint _lazer_ref 0 (select (.bblockinghit _outhit) (.location _outhit) _returnvalue_8))
              (Transformation|SetWorldLocation (Variables|Default|GetDark_Aether_Hit_Particle) (select (.bblockinghit _outhit) (.location _outhit) _returnvalue_8) false false)
              (if (.bblockinghit _outhit)
                (Utilities|IsValid (Actor|GetComponentbyClass (.hitactor _outhit) "/Game/SpyroContent/Global_Assets/Global_Components/Damageable_Com.Damageable_Com_C")
                  (:Is%20Valid
                    (Default|DealDamage (Actor|GetComponentbyClass (.hitactor _outhit) "/Game/SpyroContent/Global_Assets/Global_Components/Damageable_Com.Damageable_Com_C") "NewEnumerator4" (select (Utilities|Enum|Equal(Enum) (Variables|/Game/SpyroContent/Global_Assets/Global_Characters/Playable_Characters/BP_Base_Playable.BP_Base_Playable_C|GetPlayer_State _mycreator_2) "NewEnumerator14") (Math|Vector|GetForwardVector (Variables|/Game/SpyroContent/Global_Assets/Global_Characters/Playable_Characters/BP_Base_Playable.BP_Base_Playable_C|GetFollowCamera _mycreator_2)) (Transformation|GetActorForwardVector _mycreator_2)) true (Variables|Default|GetMyCreator) true)
                    (Utilities|FlowControl|DoOnce false
                      (:Completed
                        (Effects|SpawnEmitteratLocation "/Game/SpyroContent/Global_Assets/Global_Level_Items/Dragon_Breath/Blueprints/Aether/Particles/DarkAether_Blast.DarkAether_Blast" (select (.bblockinghit _outhit) (.location _outhit) _returnvalue_8))
                        (Audio|PlaySoundatLocation "/Game/SpyroContent/Global_Assets/Global_Level_Items/Dragon_Breath/Blueprints/Aether/Audio/dark_aether_hit_sfx.dark_aether_hit_sfx" (select (.bblockinghit _outhit) (.location _outhit) _returnvalue_8) "0, 0, 0" 1.0 1.0 0.0 0 0 0)
                        (Utilities|FlowControl|Delay 0.5)
                        (CallFunction|UnlockExplosion)))))))
            (:else)))))
    (:else)))

(event EventBeginPlay
  (bind _asspyro_persistant_data (Utilities|Casting|CastToSpyro_PersistantData (Game|GetGameInstance)))
  (EventDispatchers|BindEventtoBeginLevelTransition _asspyro_persistant_data (delegate Custom|Self%20Destruct)))

(event EventDestroyed
  (Components|DestroyComponent (Variables|Default|GetLazer_Ref)))

(fn ConstructionScript)