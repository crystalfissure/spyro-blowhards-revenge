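; Butterfly pickup that heals the player by one hit point through Sparx, the dragonfly companion.
; It bobs via randomized timelines and detects players by hitbox overlap plus a repeating sphere trace.
; When needed, or always for Blue_Butterfly_BP, it flees in circles while Sparx chases and eats it.
; It is consumed instantly at critical health or, with a sparkle, when Sparx already has a target; non-blue heals also update skill level.
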(event OnComponentBeginOverlap(Hitbox)
  (params (OverlappedComponent :type Primitive%20Component%20Object%20Reference) (OtherActor :type Actor%20Object%20Reference) (OtherComp :type Primitive%20Component%20Object%20Reference) (OtherBodyIndex :type Integer) (bFromSweep :type Boolean) (SweepResult :type Hit%20Result%20Structure%20%28by%20ref%29))
  (CallFunction|ButterflyHitboxOverlapped OtherActor OtherComp))

(event Custom|Heal%20Player
  (params (Delay%20Saving :type Boolean))
  (bind _self self)
  (bind _dragonfly_chasing_me (Variables|Default|GetDragonfly_Chasing_Me)
    (:then
      (bind _owning_player (Variables|/Game/SpyroContent/Global_Assets/Global_Characters/Sparx/Sparx_BP.Sparx_BP_C|GetOwning_Player _dragonfly_chasing_me)
        (:then
          (if (and (not (Variables|/Game/SpyroContent/Global_Assets/Global_SaveData/Spyro_PersistantData.Spyro_PersistantData_C|GetPortal_Transition (Variables|/Game/SpyroContent/Global_Assets/Global_Characters/Playable_Characters/BP_Base_Playable.BP_Base_Playable_C|GetPersData_Ref _owning_player))) (not (Utilities|Enum|Equal(Enum) (Variables|/Game/SpyroContent/Global_Assets/Global_Characters/Playable_Characters/BP_Base_Playable.BP_Base_Playable_C|GetPlayer_State _owning_player) "NewEnumerator11")))
            (Variables|/Game/SpyroContent/Global_Assets/Global_Components/Damageable_Com.Damageable_Com_C|SetHit%20Points (Variables|/Game/SpyroContent/Global_Assets/Global_Characters/Playable_Characters/BP_Base_Playable.BP_Base_Playable_C|GetDamageable _owning_player) (select (> (+ (Variables|/Game/SpyroContent/Global_Assets/Global_Components/Damageable_Com.Damageable_Com_C|GetHit%20Points (Variables|/Game/SpyroContent/Global_Assets/Global_Characters/Playable_Characters/BP_Base_Playable.BP_Base_Playable_C|GetDamageable _owning_player)) 1) (Variables|/Game/SpyroContent/Global_Assets/Global_Characters/Playable_Characters/BP_Base_Playable.BP_Base_Playable_C|GetMax_Hit_Points _owning_player)) (Variables|/Game/SpyroContent/Global_Assets/Global_Characters/Playable_Characters/BP_Base_Playable.BP_Base_Playable_C|GetMax_Hit_Points _owning_player) (+ (Variables|/Game/SpyroContent/Global_Assets/Global_Components/Damageable_Com.Damageable_Com_C|GetHit%20Points (Variables|/Game/SpyroContent/Global_Assets/Global_Characters/Playable_Characters/BP_Base_Playable.BP_Base_Playable_C|GetDamageable _owning_player)) 1)))
            (Default|SparxLimitHP _owning_player)
            (Utilities|Casting|CastToBlue_Butterfly_BP _self
              (:CastFailed
                (CallFunction|UpdateSkillLevel 7.0 _self)))))
        (:else)))
    (:else)))

(event Custom|Fly%20Down
  (bind _returnvalue (Transformation|GetActorLocation))
  (Variables|Default|SetTarget%20Height%20Offset (Math|Random|RandomFloatinRange 5.0 1e+01))
  (Variables|Default|SetHeight%20Lerp%20Alpha%20Multiplier (Math|Random|RandomFloatinRange 0.2 1.0))
  (bind _newtrack_0 (Timeline|Timeline_1 PlayFromStart)
    (:Update
      (Transformation|SetActorLocation (Math|Vector|MakeVector (.x _returnvalue) (.y _returnvalue) (Math|Float|Lerp (.z _returnvalue) (- (Variables|Default|GetTarget_Height) (Variables|Default|GetTarget%20Height%20Offset)) (* _newtrack_0 (Variables|Default|GetHeight%20Lerp%20Alpha%20Multiplier)))) true false))
    (:Finished
      (Utilities|FlowControl|Delay (Math|Random|RandomFloatinRange 0.2 1.5))
      (CallFunction|FlyUp))))

(event Custom|Fly%20Up
  (bind _returnvalue (Transformation|GetActorLocation))
  (Variables|Default|SetTarget%20Height%20Offset (Math|Random|RandomFloatinRange 5.0 1e+01))
  (Variables|Default|SetHeight%20Lerp%20Alpha%20Multiplier (Math|Random|RandomFloatinRange 0.2 1.0))
  (bind _newtrack_0 (Timeline|Timeline_0 PlayFromStart)
    (:Update
      (Transformation|SetActorLocation (Math|Vector|MakeVector (.x _returnvalue) (.y _returnvalue) (Math|Float|Lerp (.z _returnvalue) (+ (Variables|Default|GetTarget_Height) (Variables|Default|GetTarget%20Height%20Offset)) (* _newtrack_0 (Variables|Default|GetHeight%20Lerp%20Alpha%20Multiplier)))) true false))
    (:Finished
      (Utilities|FlowControl|Delay (Math|Random|RandomFloatinRange 0.2 1.5))
      (CallFunction|FlyDown))))

(event Custom|Butterfly%20Hitbox%20Overlapped
  (params (Other%20Actor :type Actor%20Object%20Reference) (Other%20Comp :type Primitive%20Component%20Object%20Reference))
  (bind _asbp_base_playable (Utilities|Casting|CastToBP_Base_Playable Other%20Actor))
  (bind _persdata_ref (Variables|/Game/SpyroContent/Global_Assets/Global_Characters/Playable_Characters/BP_Base_Playable.BP_Base_Playable_C|GetPersData_Ref _asbp_base_playable)
    (:then
      (bind _assparx_bp (Utilities|Casting|CastToSparx_BP (Variables|/Script/Engine.ChildActorComponent|GetChildActor (Variables|/Game/SpyroContent/Global_Assets/Global_Characters/Playable_Characters/BP_Base_Playable.BP_Base_Playable_C|GetSparx _asbp_base_playable))))
      (if (Math|Boolean|ANDBoolean (== (Variables|/Script/Engine.Character|GetCapsuleComponent _asbp_base_playable) Other%20Comp) (not (Variables|/Game/SpyroContent/Global_Assets/Global_SaveData/Spyro_PersistantData.Spyro_PersistantData_C|GetPortal_Transition _persdata_ref)) (not (Utilities|Enum|Equal(Enum) (Variables|/Game/SpyroContent/Global_Assets/Global_Characters/Playable_Characters/BP_Base_Playable.BP_Base_Playable_C|GetPlayer_State _asbp_base_playable) "NewEnumerator11")) (Utilities|Enum|Equal(Enum) (Variables|/Game/SpyroContent/Global_Assets/Global_Components/Base_AI_Character.Base_AI_Character_C|GetAICharacter_State (Variables|Default|GetFlying_AI_Character)) "NewEnumerator0") (Math|Boolean|ORBoolean (Utilities|Enum|Equal(Enum) (Variables|/Game/SpyroContent/Global_Assets/Global_Characters/Sparx/Sparx_BP.Sparx_BP_C|GetSparx%20State _assparx_bp) "NewEnumerator0") (Utilities|Enum|Equal(Enum) (Variables|/Game/SpyroContent/Global_Assets/Global_Characters/Sparx/Sparx_BP.Sparx_BP_C|GetSparx%20State _assparx_bp) "NewEnumerator2") (Utilities|Enum|Equal(Enum) (Variables|/Game/SpyroContent/Global_Assets/Global_Characters/Sparx/Sparx_BP.Sparx_BP_C|GetSparx%20State _assparx_bp) "NewEnumerator3")))
        (Variables|/Game/SpyroContent/Global_Assets/Global_Characters/Sparx/Sparx_BP.Sparx_BP_C|GetButterfly_Being_Chased _assparx_bp
          (:then
            (if (< (Variables|/Game/SpyroContent/Global_Assets/Global_Components/Damageable_Com.Damageable_Com_C|GetHit%20Points (Variables|/Game/SpyroContent/Global_Assets/Global_Characters/Playable_Characters/BP_Base_Playable.BP_Base_Playable_C|GetDamageable _asbp_base_playable)) (- (Variables|/Game/SpyroContent/Global_Assets/Global_Characters/Playable_Characters/BP_Base_Playable.BP_Base_Playable_C|GetMax_Hit_Points _asbp_base_playable) 1))
              _
              (else
                (Utilities|Casting|CastToBlue_Butterfly_BP self)))
            (|ManageExtraButterflies _assparx_bp))
          (:else
            (if (< (Variables|/Game/SpyroContent/Global_Assets/Global_Components/Damageable_Com.Damageable_Com_C|GetHit%20Points (Variables|/Game/SpyroContent/Global_Assets/Global_Characters/Playable_Characters/BP_Base_Playable.BP_Base_Playable_C|GetDamageable _asbp_base_playable)) (Variables|/Game/SpyroContent/Global_Assets/Global_Characters/Playable_Characters/BP_Base_Playable.BP_Base_Playable_C|GetMax_Hit_Points _asbp_base_playable))
              _
              (else
                (Utilities|Casting|CastToBlue_Butterfly_BP self)))
            (if (not (Utilities|Enum|Equal(Enum) (Variables|/Game/SpyroContent/Global_Assets/Global_Characters/Sparx/Sparx_BP.Sparx_BP_C|GetSparx%20State _assparx_bp) "NewEnumerator3"))
              (Variables|Default|SetDragonfly_Chasing_Me _assparx_bp)
              (if (<= (Variables|/Game/SpyroContent/Global_Assets/Global_Components/Damageable_Com.Damageable_Com_C|GetHit%20Points (Variables|/Game/SpyroContent/Global_Assets/Global_Characters/Playable_Characters/BP_Base_Playable.BP_Base_Playable_C|GetDamageable _asbp_base_playable)) 1)
                (CallFunction|HealPlayer false)
                (Transformation|SetWorldLocation (Variables|/Game/SpyroContent/Global_Assets/Global_Characters/Sparx/Sparx_BP.Sparx_BP_C|GetCapsule (Variables|Default|GetDragonfly_Chasing_Me)) (Transformation|GetActorLocation) false false)
                (Rendering|SetActorHiddenInGame true)
                (Variables|/Game/SpyroContent/Global_Assets/Global_Components/Base_AI_Character.Base_AI_Character_C|SetAICharacter_State (Variables|Default|GetFlying_AI_Character) "NewEnumerator2")
                (CallFunction|DelayedSelf-Destruct)
                (else
                  (Default|ChangeAICharacterState (Variables|Default|GetFlying_AI_Character) "NewEnumerator1")
                  (Variables|/Game/SpyroContent/Global_Assets/Global_Characters/Sparx/Sparx_BP.Sparx_BP_C|SetButterfly_Being_Chased _assparx_bp self)
                  (Variables|/Game/SpyroContent/Global_Assets/Global_Characters/Sparx/Sparx_BP.Sparx_BP_C|SetSparx%20State _assparx_bp "NewEnumerator3"))))))))
    (:else)))

(event Custom|Ping
  (bind _hitbox (Variables|Default|GetHitbox))
  (bind _hitbox_2 (Variables|Default|GetHitbox))
  (bind _returnvalue (Transformation|GetWorldLocation _hitbox_2))
  (bind _outhits (Collision|MultiSphereTraceForObjects _returnvalue _returnvalue (* (Variables|/Script/Engine.SphereComponent|GetSphereRadius _hitbox) (.z (Variables|/Script/Engine.SceneComponent|GetRelativeScale3D _hitbox))) (Utilities|Array|MakeArray "ObjectTypeQuery3" "ObjectTypeQuery8" "ObjectTypeQuery9") false 0 "None"))
  (for _array_element _outhits
    (CallFunction|ButterflyHitboxOverlapped (.hitactor _array_element) (.hitcomponent _array_element))))

(event Custom|Delayed%20Self-Destruct
  (Utilities|FlowControl|Delay 1.0)
  (Actor|DestroyActor))

(event EventBeginPlay
  (bind _returnvalue (Transformation|GetActorLocation))
  (bind (_x _y _z) (Math|Vector|BreakVector _returnvalue))
  (bind _asspyro_persistant_data (Utilities|Casting|CastToSpyro_PersistantData (Game|GetGameInstance)))
  (Variables|/Game/SpyroContent/Global_Assets/Global_SaveData/Spyro_PersistantData.Spyro_PersistantData_C|GetPlayer_in_Portal _asspyro_persistant_data
    (:then
      (Actor|DestroyActor))
    (:else
      (Utilities|Time|SetTimerbyFunctionName 0 "Ping" 0.5 true)
      (EventDispatchers|BindEventtoMyStateChanged (Variables|Default|GetFlying_AI_Character) (delegate OnStateChange))
      (CallFunction|OnButterflyStateChanged)
      (bind _asdropshadow_bp (Utilities|Casting|CastToDropshadow_BP (Variables|/Script/Engine.ChildActorComponent|GetChildActor (Variables|Default|GetDropshadow))))
      (Variables|/Game/SpyroContent/Global_Assets/Global_Level_Items/Dropshadow/Dropshadow_BP.Dropshadow_BP_C|SetOwning%20Component _asdropshadow_bp (Variables|Default|GetStaticMesh))
      (bind _outhit (Collision|LineTraceForObjects _returnvalue (Math|Vector|MakeVector _x _y (- _z 1e+02)) (Utilities|Array|MakeArray "ObjectTypeQuery1") false 0 "None"))
      (if (.bblockinghit _outhit)
        (Variables|Default|SetTarget_Height (+ (.Z (Math|Vector|BreakVector (.location _outhit))) 8e+01))
        (else
          (Variables|Default|SetTarget_Height (.z (Transformation|GetActorLocation)))))
      (CallFunction|FlyUp))))

(event EventTick
  (params (DeltaSeconds :type Float%20%28single-precision%29))
  (if (Utilities|Enum|Equal(Enum) (Variables|/Game/SpyroContent/Global_Assets/Global_Components/Base_AI_Character.Base_AI_Character_C|GetAICharacter_State (Variables|Default|GetFlying_AI_Character)) "NewEnumerator1")
    (Transformation|AddActorWorldOffset (* (Transformation|GetActorForwardVector) (* (Utilities|Time|GetWorldDeltaSeconds) (* (Variables|/Game/SpyroContent/Global_Assets/Global_Components/Child_Components/Flying_AI_Character.Flying_AI_Character_C|GetFlyingSpeed (Variables|Default|GetFlying_AI_Character)) 4.0))) true)
    (bind _returnvalue (Default|IsThisActorStuck? (Variables|Default|GetFlying_AI_Character)))
    (if _returnvalue
      (Transformation|AddActorLocalRotation (Math|Rotator|MakeRotator 0.0 0.0 (* (Utilities|Time|GetWorldDeltaSeconds) 3e+03)) false false)
      (elif (Variables|Default|GetFlying%20in%20Circles)
        (Transformation|AddActorLocalRotation (Math|Rotator|MakeRotator 0.0 0.0 (* (Utilities|Time|GetWorldDeltaSeconds) 2e+02 (select (Variables|Default|GetCounterclockwise) -1.0 1.0))) false false)))))

(fn ConstructionScript)

(event Custom|On%20Butterfly%20State%20Changed
  (bind _returnvalue (Transformation|GetActorLocation))
  (bind _dragonfly_chasing_me (Variables|Default|GetDragonfly_Chasing_Me))
  (bind _dragonfly_chasing_me_2 (Variables|Default|GetDragonfly_Chasing_Me))
  (bind _mesh (Variables|/Game/SpyroContent/Global_Assets/Global_Characters/Sparx/Sparx_BP.Sparx_BP_C|GetMesh _dragonfly_chasing_me))
  (bind _returnvalue_2 (Transformation|GetWorldLocation _mesh))
  (bind _returnvalue_3 (Math|Rotator|FindLookatRotation _returnvalue _returnvalue_2))
  (switch Utilities|FlowControl|Switch|SwitchonAICharacter_States (Variables|/Game/SpyroContent/Global_Assets/Global_Components/Base_AI_Character.Base_AI_Character_C|GetAICharacter_State (Variables|Default|GetFlying_AI_Character))
    (:NewEnumerator1
      (Variables|Default|SetCounterclockwise (Math|Random|RandomBool))
      (Utilities|FlowControl|Delay 0.2)
      (Default|StarttheStuckPreventionTimer (Variables|Default|GetFlying_AI_Character) 0.1)
      (Transformation|SetActorRotation (Math|Rotator|MakeRotator (.roll _returnvalue_3) (.pitch _returnvalue_3) (+ (.yaw _returnvalue_3) 1.8e+02)))
      (Variables|Default|SetFlying%20in%20Circles true)
      (Utilities|FlowControl|Delay 0.5)
      (Utilities|FlowControl|Delay 0.8)
      (Variables|/Game/SpyroContent/Global_Assets/Global_Characters/Sparx/Sparx_BP.Sparx_BP_C|SetEating_Butterfly _dragonfly_chasing_me_2 true)
      (bind _assparx_abp (Utilities|Casting|CastToSparx_ABP (Components|SkeletalMesh|GetAnimInstance (Variables|/Game/SpyroContent/Global_Assets/Global_Characters/Sparx/Sparx_BP.Sparx_BP_C|GetMesh _dragonfly_chasing_me_2))))
      (Variables|/Game/SpyroContent/Global_Assets/Global_Characters/Sparx/Sparx_ABP.Sparx_ABP_C|SetABP_Eating_Butterfly _assparx_abp true))))