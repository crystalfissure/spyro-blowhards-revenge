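; Blue butterfly collectible, a child Blueprint that fully heals the player whose dragonfly chases it and grants an extra life.
; HealPlayer skips portal transitions and one excluded player state, refills hit points, then passes the level item index to the controller's GainALife.
; It saves itself as a collected item in persistent data and updates skill level.
; Saving and delayed self-destruct retry until a unique name and valid index are assigned.
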(event Custom|check%20again
  (if (or (Utilities|Enum|Equal(Enum) (Variables|Default|GetMy_Unique_Name) "DEFAULT") (< (Variables|Default|GetLevel%20Item%20Index) 0))
    (Utilities|FlowControl|Delay 0.2)
    (CallFunction|CheckAgain)
    (else
      (Actor|DestroyActor))))

(event Custom|do%20i%20have%20a%20name%20yet?
  (if (or (Utilities|Enum|Equal(Enum) (Variables|Default|GetMy_Unique_Name) "DEFAULT") (< (Variables|Default|GetLevel%20Item%20Index) 0))
    (Utilities|FlowControl|Delay 0.2)
    (CallFunction|DoIHaveANameYet?)
    (else
      (bind _asspyro_player_controller (Utilities|Casting|CastToSpyro_PlayerController (Pawn|GetController (stale EventHealPlayer _owning_player)))
        (:then
          (Default|GainALife _asspyro_player_controller (Variables|Default|GetLevel%20Item%20Index)))
        (:CastFailed
          _))
      (if (stale EventHealPlayer Delay%20Saving)
        (Utilities|FlowControl|Delay 0.2))
      (if (Utilities|Enum|Equal(Enum) (Variables|Default|GetMy_Unique_Name) "DEFAULT")
        (Development|PrintString "FAILED TO SAVE BLUE BUTTERFLY DUE TO LACKING A UNIQUE NAME. WAS IT SPAWNED IN PROPERLY?")
        (else
          (bind _asspyro_persistant_data (Utilities|Casting|CastToSpyro_PersistantData (Game|GetGameInstance)))
          (Default|SaveACollectible _asspyro_persistant_data "NewEnumerator2" (Variables|Default|GetMy_Unique_Name) 0.0 (Variables|Default|GetLevel%20Item%20Index) 0.0)
          (Default|CallSavedACollectable)
          (CallFunction|UpdateSkillLevel (Variables|Default|GetSkill%20Level%20Award) self))))))

(event EventDelayedSelf-Destruct
  (Utilities|FlowControl|Delay 1.0)
  (if (or (Utilities|Enum|Equal(Enum) (Variables|Default|GetMy_Unique_Name) "DEFAULT") (< (Variables|Default|GetLevel%20Item%20Index) 0))
    (Utilities|FlowControl|Delay 0.2)
    (CallFunction|CheckAgain)
    (else
      (Actor|DestroyActor))))

(event EventHealPlayer
  (params (Delay%20Saving :type Boolean))
  (bind _dragonfly_chasing_me (Variables|Default|GetDragonfly_Chasing_Me)
    (:then
      (bind _owning_player (Variables|/Game/SpyroContent/Global_Assets/Global_Characters/Sparx/Sparx_BP.Sparx_BP_C|GetOwning_Player _dragonfly_chasing_me)
        (:then
          (if (and (not (Variables|/Game/SpyroContent/Global_Assets/Global_SaveData/Spyro_PersistantData.Spyro_PersistantData_C|GetPortal_Transition (Variables|/Game/SpyroContent/Global_Assets/Global_Characters/Playable_Characters/BP_Base_Playable.BP_Base_Playable_C|GetPersData_Ref _owning_player))) (not (Utilities|Enum|Equal(Enum) (Variables|/Game/SpyroContent/Global_Assets/Global_Characters/Playable_Characters/BP_Base_Playable.BP_Base_Playable_C|GetPlayer_State _owning_player) "NewEnumerator11")))
            (Variables|/Game/SpyroContent/Global_Assets/Global_Components/Damageable_Com.Damageable_Com_C|SetHit%20Points (Variables|/Game/SpyroContent/Global_Assets/Global_Characters/Playable_Characters/BP_Base_Playable.BP_Base_Playable_C|GetDamageable _owning_player) (Variables|/Game/SpyroContent/Global_Assets/Global_Characters/Playable_Characters/BP_Base_Playable.BP_Base_Playable_C|GetMax_Hit_Points _owning_player))
            (Default|SparxLimitHP _owning_player)
            (if (or (Utilities|Enum|Equal(Enum) (Variables|Default|GetMy_Unique_Name) "DEFAULT") (< (Variables|Default|GetLevel%20Item%20Index) 0))
              (Utilities|FlowControl|Delay 0.2)
              (CallFunction|DoIHaveANameYet?)
              (else
                (bind _asspyro_player_controller (Utilities|Casting|CastToSpyro_PlayerController (Pawn|GetController _owning_player))
                  (:then
                    (Default|GainALife _asspyro_player_controller (Variables|Default|GetLevel%20Item%20Index)))
                  (:CastFailed
                    _))
                (if Delay%20Saving
                  (Utilities|FlowControl|Delay 0.2))
                (if (Utilities|Enum|Equal(Enum) (Variables|Default|GetMy_Unique_Name) "DEFAULT")
                  (Development|PrintString "FAILED TO SAVE BLUE BUTTERFLY DUE TO LACKING A UNIQUE NAME. WAS IT SPAWNED IN PROPERLY?")
                  (else
                    (bind _asspyro_persistant_data (Utilities|Casting|CastToSpyro_PersistantData (Game|GetGameInstance)))
                    (Default|SaveACollectible _asspyro_persistant_data "NewEnumerator2" (Variables|Default|GetMy_Unique_Name) 0.0 (Variables|Default|GetLevel%20Item%20Index) 0.0)
                    (Default|CallSavedACollectable)
                    (CallFunction|UpdateSkillLevel (Variables|Default|GetSkill%20Level%20Award) self)))))))
        (:else)))
    (:else)))

(fn ConstructionScript
  (|CallParentFunction))