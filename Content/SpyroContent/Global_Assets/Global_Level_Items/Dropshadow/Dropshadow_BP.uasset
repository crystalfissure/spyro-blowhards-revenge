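; Drop shadow actor that sits on the ground beneath the component it is assigned to.
; Each tick it traces straight down from the owning component against WorldStatic objects, ignoring that component's owner, and moves itself just above the hit point.
; It hides when the hit is a BP_KillPlane and reappears over other surfaces; with no hit, it keeps its last position and visibility.
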(event EventTick
  (params (DeltaSeconds :type Float%20%28single-precision%29))
  (bind _owning_component (Variables|Default|GetOwning%20Component)
    (:then
      (bind _outhit (Collision|LineTraceForObjects (Transformation|GetWorldLocation _owning_component) (Math|Vector|MakeVector (.X (Math|Vector|BreakVector (Transformation|GetWorldLocation _owning_component))) (.Y (Math|Vector|BreakVector (Transformation|GetWorldLocation _owning_component))) (- (.Z (Math|Vector|BreakVector (Transformation|GetWorldLocation _owning_component))) 9999.0)) (Utilities|Array|MakeArray "ObjectTypeQuery1") false (Utilities|Array|MakeArray (Components|GetOwner (Variables|Default|GetOwning%20Component))) "None"))
      (if (.bblockinghit _outhit)
        (Utilities|Casting|CastToBP_KillPlane (.hitactor _outhit)
          (:then
            (if (not (Variables|Rendering|GetbHidden))
              (Rendering|SetActorHiddenInGame true)))
          (:CastFailed
            (Transformation|SetActorLocation (Math|Vector|MakeVector (.X (Math|Vector|BreakVector (.location _outhit))) (.Y (Math|Vector|BreakVector (.location _outhit))) (+ (.Z (Math|Vector|BreakVector (.location _outhit))) 5.0)) false false)
            (if (Variables|Rendering|GetbHidden)
              (Rendering|SetActorHiddenInGame false))))))
    (:else)))

(fn ConstructionScript)