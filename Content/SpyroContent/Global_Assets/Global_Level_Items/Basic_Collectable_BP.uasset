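; Basic collectable level item that saves itself as collected when a playable character touches it, then destroys itself.
; The hitbox overlap only counts the BP_Base_Playable capsule component.
; It passes the NPCAwardItem level item index and a fixed skill award to SaveACollectible on the Spyro_PersistantData game instance.
; Pickup particle and sound nodes are unwired placeholders, as are the level setup and collected-item cleanup calls.
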(event OnComponentBeginOverlap(Hitbox)
  (params (OverlappedComponent :type Primitive%20Component%20Object%20Reference) (OtherActor :type Actor%20Object%20Reference) (OtherComp :type Primitive%20Component%20Object%20Reference) (OtherBodyIndex :type Integer) (bFromSweep :type Boolean) (SweepResult :type Hit%20Result%20Structure%20%28by%20ref%29))
  (bind _asbp_base_playable (Utilities|Casting|CastToBP_Base_Playable OtherActor))
  (if (== (Variables|/Script/Engine.Character|GetCapsuleComponent _asbp_base_playable) OtherComp)
    (bind _asspyro_persistant_data (Utilities|Casting|CastToSpyro_PersistantData (Game|GetGameInstance)))
    (Default|SaveACollectible _asspyro_persistant_data "NewEnumerator1" "" 0.0 (Variables|/Game/SpyroContent/Global_Assets/Global_Components/NPC_Award_Item.NPC_Award_Item_C|GetLevel%20Item%20Index (Variables|Default|GetNPC_Award_Item)) 5.0)
    (Actor|DestroyActor)))

(fn ConstructionScript)