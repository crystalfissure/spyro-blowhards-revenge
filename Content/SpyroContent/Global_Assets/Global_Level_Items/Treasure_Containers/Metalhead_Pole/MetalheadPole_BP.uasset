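; Metalhead pole treasure container that periodically electrifies while players are near, hurting them on contact.
; An awake-radius overlap tracks players and runs a looping countdown timer that cycles Green, Blinking warning and Red states, resetting to Green once the radius empties.
; Each state change updates the dynamic material, damage resistances, capsule collision, electricity mesh and audio.
; Successfully damaging the container returns it to Green, and destruction halts the cycle.
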(event OnComponentBeginOverlap(Awake_Radius)
  (params (OverlappedComponent :type Primitive%20Component%20Object%20Reference) (OtherActor :type Actor%20Object%20Reference) (OtherComp :type Primitive%20Component%20Object%20Reference) (OtherBodyIndex :type Integer) (bFromSweep :type Boolean) (SweepResult :type Hit%20Result%20Structure%20%28by%20ref%29))
  (bind _asbp_base_playable (Utilities|Casting|CastToBP_Base_Playable OtherActor))
  (if (== (Variables|/Script/Engine.Character|GetCapsuleComponent _asbp_base_playable) OtherComp)
    (Utilities|Array|AddUnique (Variables|Default|GetPlayers%20in%20My%20Radius) _asbp_base_playable)
    (if (and (> (Utilities|Array|Length (Variables|Default|GetPlayers%20in%20My%20Radius)) 0) (not (Utilities|Time|IsValidTimerHandle (Variables|Default|GetCountdown%20Timer))))
      (Utilities|Time|ClearandInvalidateTimerbyHandle (Variables|Default|GetCountdown%20Timer))
      (bind _returnvalue (Utilities|Time|SetTimerbyFunctionName 0 "Countdown" 0.5 true))
      (Variables|Default|SetCountdown%20Timer _returnvalue))))

(event OnComponentEndOverlap(Awake_Radius)
  (params (OverlappedComponent :type Primitive%20Component%20Object%20Reference) (OtherActor :type Actor%20Object%20Reference) (OtherComp :type Primitive%20Component%20Object%20Reference) (OtherBodyIndex :type Integer))
  (bind _players_in_my_radius (Variables|Default|GetPlayers%20in%20My%20Radius))
  (bind _asbp_base_playable (Utilities|Casting|CastToBP_Base_Playable OtherActor))
  (if (== (Variables|/Script/Engine.Character|GetCapsuleComponent _asbp_base_playable) OtherComp)
    (Utilities|Array|RemoveItem _players_in_my_radius _asbp_base_playable)
    (if (<= (Utilities|Array|Length _players_in_my_radius) 0)
      (Utilities|Time|ClearandInvalidateTimerbyHandle (Variables|Default|GetCountdown%20Timer))
      (Variables|Default|SetCountdown%20to%20Switch (.Countdown%20to%20Switch (Utilities|GetClassDefaults "MetalheadPole_BP_C")))
      (CallFunction|ChangeMetalheadPoleState "NewEnumerator0"))))

(event OnComponentHit(CapsuleComponent)
  (params (HitComponent :type Primitive%20Component%20Object%20Reference) (OtherActor :type Actor%20Object%20Reference) (OtherComp :type Primitive%20Component%20Object%20Reference) (NormalImpulse :type Vector :default "0, 0, 0") (Hit :type Hit%20Result%20Structure%20%28by%20ref%29))
  (bind _asbp_base_playable (Utilities|Casting|CastToBP_Base_Playable OtherActor))
  (if (and (== (Variables|/Script/Engine.Character|GetCapsuleComponent _asbp_base_playable) OtherComp) (Utilities|Enum|Equal(Enum) (Variables|Default|GetMealhead%20Pole%20State) "NewEnumerator1"))
    (Default|DealDamage (Variables|/Game/SpyroContent/Global_Assets/Global_Characters/Playable_Characters/BP_Base_Playable.BP_Base_Playable_C|GetDamageable _asbp_base_playable) "NewEnumerator3" "0, 0, 0" false _asbp_base_playable false)))

(event EventBeginPlay
  (bind _awake_radius (Variables|Default|GetAwake_Radius))
  (bind _returnvalue (Transformation|GetWorldLocation _awake_radius))
  (|CallParentFunction)
  (Variables|/Game/SpyroContent/Global_Assets/Global_Components/Damageable_Com.Damageable_Com_C|SetComponent_with_Metal_Material (Variables|Default|GetDamageable) (Variables|Default|GetStaticMesh))
  (bind _returnvalue_2 (Rendering|Material|CreateDynamicMaterialInstance (Variables|Default|GetStaticMesh) 2 "/Game/SpyroContent/Global_Assets/Global_Materials/Material_Instances/Untex_Vertex_Color.Untex_Vertex_Color" "None" :!class /Script/Engine.PrimitiveComponent))
  (bind _output_get (Variables|Default|SetDynMat%20Ref _returnvalue_2))
  (Rendering|Material|SetVectorParameterValue _output_get "ColorChange" (Variables|Default|GetGreenColor) :!class /Script/Engine.MaterialInstanceDynamic)
  (Rendering|Material|SetVectorParameterValue (Variables|Default|GetDynMat%20Ref) "ColorChange2" "(R=1.000000,G=0.000000,B=0.043137,A=1.000000)" :!class /Script/Engine.MaterialInstanceDynamic)
  (Rendering|Material|SetScalarParameterValue (Variables|Default|GetDynMat%20Ref) "Blink Duration" 0.3 :!class /Script/Engine.MaterialInstanceDynamic)
  (bind _outhits (Collision|MultiSphereTraceForObjects _returnvalue _returnvalue (Variables|/Script/Engine.SphereComponent|GetSphereRadius _awake_radius) (Utilities|Array|MakeArray "ObjectTypeQuery3" "ObjectTypeQuery8" "ObjectTypeQuery9" "ObjectTypeQuery10") false 0 "None"))
  (for _array_element _outhits
    (bind _asbp_base_playable (Utilities|Casting|CastToBP_Base_Playable (.hitactor _array_element)))
    (if (== (Variables|/Script/Engine.Character|GetCapsuleComponent _asbp_base_playable) (.hitcomponent _array_element))
      (Utilities|Array|AddUnique (Variables|Default|GetPlayers%20in%20My%20Radius) _asbp_base_playable)
      (if (and (> (Utilities|Array|Length (Variables|Default|GetPlayers%20in%20My%20Radius)) 0) (not (Utilities|Time|IsValidTimerHandle (Variables|Default|GetCountdown%20Timer))))
        (Utilities|Time|ClearandInvalidateTimerbyHandle (Variables|Default|GetCountdown%20Timer))
        (bind _returnvalue_3 (Utilities|Time|SetTimerbyFunctionName 0 "Countdown" 0.5 true))
        (Variables|Default|SetCountdown%20Timer _returnvalue_3)))))

(event EventTreasureContainerSuccessfullyDamaged
  (|CallParentFunction)
  (CallFunction|ChangeMetalheadPoleState "NewEnumerator0"))

(fn ConstructionScript
  (|CallParentFunction))

(fn Countdown
  (if (not (Variables|Default|GetContainer_Destroyed))
    (bind _output_get (Variables|Default|SetCountdown%20to%20Switch (select (>= (- (Variables|Default|GetCountdown%20to%20Switch) 1) 0) (- (Variables|Default|GetCountdown%20to%20Switch) 1) 0)))
    (if (<= _output_get 2)
      (if (<= (Variables|Default|GetCountdown%20to%20Switch) 0)
        (CallFunction|ChangeMetalheadPoleState (Utilities|Select :Index (Variables|Default|GetMealhead%20Pole%20State) :NewEnumerator0 "NewEnumerator1" :NewEnumerator1 "NewEnumerator0" :NewEnumerator2 "NewEnumerator1"))
        (elif (and (Utilities|Enum|Equal(Enum) (Variables|Default|GetMealhead%20Pole%20State) "NewEnumerator0") (<= (Variables|Default|GetCountdown%20to%20Switch) 2))
          (CallFunction|ChangeMetalheadPoleState "NewEnumerator2"))))))

(fn ChangeMetalheadPoleState
  (params (Mealhead%20Pole%20State :type MetalheadPole_Enum%20Enum :default "NewEnumerator0"))
  (bind _array (Utilities|Array|MakeArray "NewEnumerator1" "NewEnumerator9" "NewEnumerator10" "NewEnumerator11" "NewEnumerator13" "NewEnumerator7"))
  (bind _greencolor (Variables|Default|GetGreenColor))
  (if (not (Utilities|Enum|Equal(Enum) Mealhead%20Pole%20State (Variables|Default|GetMealhead%20Pole%20State)))
    (Variables|Default|SetMealhead%20Pole%20State Mealhead%20Pole%20State)
    (Rendering|Material|SetVectorParameterValue (Variables|Default|GetDynMat%20Ref) "ColorChange" (Utilities|Select :Index (Variables|Default|GetMealhead%20Pole%20State) :NewEnumerator0 _greencolor :NewEnumerator1 "(R=1.000000,G=0.000000,B=0.043137,A=1.000000)" :NewEnumerator2 _greencolor) :!class /Script/Engine.MaterialInstanceDynamic)
    (Rendering|Material|SetScalarParameterValue (Variables|Default|GetDynMat%20Ref) "Blinking Color Change?" (select (Utilities|Enum|Equal(Enum) (Variables|Default|GetMealhead%20Pole%20State) "NewEnumerator2") 1.0 0.0) :!class /Script/Engine.MaterialInstanceDynamic)
    (Variables|/Game/SpyroContent/Global_Assets/Global_Components/Damageable_Com.Damageable_Com_C|SetDamage_Resistances (Variables|Default|GetDamageable) (Utilities|Select :Index (Variables|Default|GetMealhead%20Pole%20State) :NewEnumerator0 _array :NewEnumerator1 (Utilities|Array|MakeArray "NewEnumerator1" "NewEnumerator2" "NewEnumerator4" "NewEnumerator9" "NewEnumerator10" "NewEnumerator11" "NewEnumerator13" "NewEnumerator7") :NewEnumerator2 _array))
    (Collision|SetCollisionResponsetoChannel (Variables|Default|GetCapsule%20Component) "ECC_GameTraceChannel4" (Utilities|Select :Index (Variables|Default|GetMealhead%20Pole%20State) :NewEnumerator0 "ECR_Overlap" :NewEnumerator1 "ECR_Block" :NewEnumerator2 "ECR_Overlap"))
    (Rendering|SetVisibility (Variables|Default|GetElectricity_Mesh) (Utilities|Select :Index (Variables|Default|GetMealhead%20Pole%20State) :NewEnumerator0 false :NewEnumerator1 true :NewEnumerator2 false) false)
    (Components|Activation|SetActive (Variables|Default|GetAudio) (Utilities|Select :Index (Variables|Default|GetMealhead%20Pole%20State) :NewEnumerator0 false :NewEnumerator1 true :NewEnumerator2 false) false)
    (if (and (Utilities|Enum|Equal(Enum) (Variables|Default|GetMealhead%20Pole%20State) "NewEnumerator0") (not (Variables|Default|GetContainer_Destroyed)))
      (Audio|PlaySoundatLocation "/Game/SpyroContent/Global_Assets/Global_Level_Items/Treasure_Containers/Metalhead_Pole/Audio/metalhead_pole_ending.metalhead_pole_ending" (Transformation|GetActorLocation) "0, 0, 0" 1.0 1.0 0.0 0 0 0))
    (if (or (Utilities|Enum|Equal(Enum) (Variables|Default|GetMealhead%20Pole%20State) "NewEnumerator1") (Utilities|Enum|Equal(Enum) (Variables|Default|GetMealhead%20Pole%20State) "NewEnumerator0"))
      (Variables|Default|SetCountdown%20to%20Switch (.Countdown%20to%20Switch (Utilities|GetClassDefaults "MetalheadPole_BP_C"))))))