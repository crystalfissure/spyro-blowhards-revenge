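; Spring Chest treasure container holding a child-actor gem, with chest materials matched to gem value and treasure skin.
; Resisted hits spring the gem up on a timeline, briefly making it collectable; collecting it breaks the chest with super damage.
; Successful damage either collects the gem outright or launches it with physics, magnetizing it to a nearby attacker found by sphere trace.
; Gem-reset events restore the container unless its gem state blocks it.
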(event Custom|Start%20Springing
  (|Spring))

(event Custom|On%20Gem%20Collected
  (Default|DealDamage (Variables|Default|GetDamageable) "NewEnumerator0" "0, 0, 0" true 0 false)
  (Variables|Default|SetGem%20is%20Springing false)
  (Audio|Components|Audio|Stop (Variables|Default|GetSpringChest_Audio))
  (Components|Activation|Deactivate (Variables|Default|GetParticleSystem)))

(event Custom|My%20Gem%20Unhidden
  (Rendering|SetActorHiddenInGame false))

(event Custom|On%20Gems%20Reset
  (CallFunction|ResetThisContainer))

(event Custom|On%20Gem%20Destroyed
  (params (DestroyedActor :type Actor%20Object%20Reference))
  (Rendering|SetActorHiddenInGame true)
  (Utilities|FlowControl|Delay 0.2)
  (Actor|DestroyActor))

(event Custom|On%20Treasure%20Skin%20Changed
  (bind _asgem_base_bp (Utilities|Casting|CastToGem_Base_BP (Variables|/Script/Engine.ChildActorComponent|GetChildActor (Variables|Default|GetChildActor)))
    (:then
      (Components|StaticMesh|SetStaticMesh (Variables|/Game/SpyroContent/Global_Assets/Global_Level_Items/Gems/Actors/Gem_Base_BP.Gem_Base_BP_C|GetVisual_Mesh _asgem_base_bp) "/Game/SpyroContent/Global_Assets/Global_Level_Items/Gems/Static_Meshes/gem_s1.gem_s1"))
    (:CastFailed
      _))
  (CallFunction|ManageGem'sFloatingAppearance (Variables|Default|GetChildActor) self)
  (CallFunction|SetSpringChestMat))

(event EventBeginPlay
  (bind _staticmesh (Variables|Default|GetStaticMesh))
  (bind _item_drop_component (Variables|Default|GetItem_Drop_Component))
  (bind _returnvalue (Transformation|GetWorldLocation _staticmesh))
  (bind _items_to_drop (Variables|/Game/SpyroContent/Global_Assets/Global_Components/Drops_Items.Drops_Items_C|GetItems_to_Drop _item_drop_component))
  (|CallParentFunction)
  (Utilities|Array|Clear _items_to_drop)
  (Utilities|Array|SetArrayElem _items_to_drop 0 "/Game/SpyroContent/Global_Assets/Global_Level_Items/Treasure_Containers/Dummy_Item_BP.Dummy_Item_BP_C" true)
  (CallFunction|ToggleGemCollission false)
  (CallFunction|SetSpringChestMat)
  (bind _asgem_base_bp (Utilities|Casting|CastToGem_Base_BP (Variables|/Script/Engine.ChildActorComponent|GetChildActor (Variables|Default|GetChildActor)))
    (:then
      (Transformation|AttachComponentToComponent (Variables|Default|GetParticleSystem) (Variables|/Game/SpyroContent/Global_Assets/Global_Level_Items/Gems/Actors/Gem_Base_BP.Gem_Base_BP_C|GetVisual_Mesh _asgem_base_bp) "None" "SnapToTarget" "SnapToTarget" "SnapToTarget" false)
      (Variables|/Game/SpyroContent/Global_Assets/Global_Level_Items/Gems/Actors/Gem_Base_BP.Gem_Base_BP_C|SetFloating _asgem_base_bp true)
      (Variables|/Game/SpyroContent/Global_Assets/Global_Level_Items/Gems/Actors/Gem_Base_BP.Gem_Base_BP_C|SetSparx_Cant_Grab_Me _asgem_base_bp true)
      (Physics|SetSimulatePhysics (Variables|/Game/SpyroContent/Global_Assets/Global_Level_Items/Gems/Actors/Gem_Base_BP.Gem_Base_BP_C|GetCollision_Mesh _asgem_base_bp) false)
      (bind _asspyro_persistant_data (Utilities|Casting|CastToSpyro_PersistantData (Game|GetGameInstance))
        (:then
          (EventDispatchers|BindEventtoChangeTreasureSkins _asspyro_persistant_data (delegate Custom|On%20Treasure%20Skin%20Changed)))
        (:CastFailed
          _))
      (EventDispatchers|BindEventtoDamageWasAttemptedButI'mResistant (Variables|Default|GetDamageable) (delegate Custom|Start%20Springing))
      (Game|BindEventtoOnDestroyed (delegate Custom|On%20Gem%20Destroyed))
      (EventDispatchers|BindEventtoGemWasUnhidden _asgem_base_bp (delegate Custom|My%20Gem%20Unhidden))
      (EventDispatchers|BindEventtoGemWasCollected _asgem_base_bp (delegate Custom|On%20Gem%20Collected))
      (Rendering|SetVisibility (Variables|/Game/SpyroContent/Global_Assets/Global_Level_Items/Gems/Actors/Gem_Base_BP.Gem_Base_BP_C|GetDropshadow _asgem_base_bp) false false)
      (EventDispatchers|BindEventtoResetGems _asspyro_persistant_data (delegate Custom|On%20Gems%20Reset))
      (Utilities|FlowControl|Delay 0.4)
      (bind _childactor (Variables|/Script/Engine.ChildActorComponent|GetChildActor (Variables|Default|GetChildActor))
        (:then
          (bind _asgem_base_bp_2 (Utilities|Casting|CastToGem_Base_BP _childactor)
            (:then
              (Components|StaticMesh|SetStaticMesh (Variables|/Game/SpyroContent/Global_Assets/Global_Level_Items/Gems/Actors/Gem_Base_BP.Gem_Base_BP_C|GetVisual_Mesh _asgem_base_bp_2) "/Game/SpyroContent/Global_Assets/Global_Level_Items/Gems/Static_Meshes/gem_s1.gem_s1"))
            (:CastFailed
              _))
          (CallFunction|ManageGem'sFloatingAppearance (Variables|Default|GetChildActor) self)
          (Transformation|SetActorLocation _asgem_base_bp_2 (Math|Vector|MakeVector (.x _returnvalue) (.y _returnvalue) (+ (.z _returnvalue) 24.0)) false false))
        (:else
          (Actor|DestroyActor))))
    (:CastFailed
      (Development|PrintString "Spring Chest BP: My child actor is not a gem?????" true true "(R=0.000000,G=0.660000,B=1.000000,A=1.000000)" 2e+01)
      (Actor|DestroyActor))))

(event EventTreasureContainerSuccessfullyDamaged
  (bind _damageable (Variables|Default|GetDamageable))
  (|CallParentFunction)
  (bind _asgem_base_bp (Utilities|Casting|CastToGem_Base_BP (Variables|/Script/Engine.ChildActorComponent|GetChildActor (Variables|Default|GetChildActor))))
  (if (not (Utilities|Enum|Equal(Enum) (Variables|/Game/SpyroContent/Global_Assets/Global_Level_Items/Gems/Actors/Gem_Base_BP.Gem_Base_BP_C|GetGem_State _asgem_base_bp) "NewEnumerator2"))
    (Components|Activation|Deactivate (Variables|Default|GetParticleSystem))
    (if (or (Utilities|Enum|Equal(Enum) (Variables|/Game/SpyroContent/Global_Assets/Global_Components/Damageable_Com.Damageable_Com_C|GetDeal%20Damage%20-%20Damage%20Type _damageable) "NewEnumerator4") (Variables|/Game/SpyroContent/Global_Assets/Global_Components/Damageable_Com.Damageable_Com_C|GetDeal%20Damage%20-%20Magnetize%20Immediately _damageable))
      (bind _deal_damage___person_who_dealt_the_damage (Variables|/Game/SpyroContent/Global_Assets/Global_Components/Damageable_Com.Damageable_Com_C|GetDeal%20Damage%20-%20Person%20Who%20Dealt%20the%20Damage (Variables|Default|GetDamageable))
        (:then
          (bind _asbp_base_playable (Utilities|Casting|CastToBP_Base_Playable _deal_damage___person_who_dealt_the_damage)
            (:then
              (bind _spyrocontr_ref (Variables|/Game/SpyroContent/Global_Assets/Global_Characters/Playable_Characters/BP_Base_Playable.BP_Base_Playable_C|GetSpyroContr_Ref _asbp_base_playable)
                (:then
                  (Default|CollectGem _asgem_base_bp (Variables|/Game/SpyroContent/Global_Assets/Global_Characters/Playable_Characters/Spyro_PlayerController.Spyro_PlayerController_C|GetPlayer_Index_Number _spyrocontr_ref)))
                (:else
                  (Default|CollectGem _asgem_base_bp :!label _label))))
            (:CastFailed
              (goto _label))))
        (:else
          (goto _label)))
      (else
        (Default|SetSkin _asgem_base_bp)
        (bind _asgem_base_bp_2 (Utilities|Casting|CastToGem_Base_BP (Variables|/Script/Engine.ChildActorComponent|GetChildActor (Variables|Default|GetChildActor)))
          (:then
            (Components|StaticMesh|SetStaticMesh (Variables|/Game/SpyroContent/Global_Assets/Global_Level_Items/Gems/Actors/Gem_Base_BP.Gem_Base_BP_C|GetVisual_Mesh _asgem_base_bp_2) "/Game/SpyroContent/Global_Assets/Global_Level_Items/Gems/Static_Meshes/gem_s1.gem_s1"))
          (:CastFailed
            _))
        (Default|ChangeGemState _asgem_base_bp "NewEnumerator4")
        (CallFunction|ToggleGemCollission true)
        (Physics|SetSimulatePhysics (Variables|/Game/SpyroContent/Global_Assets/Global_Level_Items/Gems/Actors/Gem_Base_BP.Gem_Base_BP_C|GetCollision_Mesh _asgem_base_bp) true)
        (Physics|SetEnableGravity (Variables|/Game/SpyroContent/Global_Assets/Global_Level_Items/Gems/Actors/Gem_Base_BP.Gem_Base_BP_C|GetCollision_Mesh _asgem_base_bp) true)
        (Rendering|SetVisibility (Variables|/Game/SpyroContent/Global_Assets/Global_Level_Items/Gems/Actors/Gem_Base_BP.Gem_Base_BP_C|GetDropshadow _asgem_base_bp) true false)
        (Collision|SetCollisionEnabled (Variables|/Game/SpyroContent/Global_Assets/Global_Level_Items/Gems/Actors/Gem_Base_BP.Gem_Base_BP_C|GetCollision_Mesh _asgem_base_bp) "QueryAndPhysics")
        (Physics|AddImpulse (Variables|/Game/SpyroContent/Global_Assets/Global_Level_Items/Gems/Actors/Gem_Base_BP.Gem_Base_BP_C|GetCollision_Mesh _asgem_base_bp) "0, 0,600.000000" "None" true)
        (Utilities|FlowControl|Delay 0.1)
        (if (Variables|Default|GetContainer_Destroyed)
          (Utilities|FlowControl|Sequence
            (:then_0
              (bind _asspyro_persistant_data (Utilities|Casting|CastToSpyro_PersistantData (Game|GetGameInstance)))
              (Variables|/Game/SpyroContent/Global_Assets/Global_SaveData/Spyro_PersistantData.Spyro_PersistantData_C|GetPlayer_in_Portal _asspyro_persistant_data
                (:then
                  (Actor|DestroyActor))
                (:else
                  (bind _asgem_base_bp_3 (Utilities|Casting|CastToGem_Base_BP (Variables|/Script/Engine.ChildActorComponent|GetChildActor (Variables|Default|GetChildActor))))
                  (if (and (not (Utilities|Enum|Equal(Enum) (Variables|/Game/SpyroContent/Global_Assets/Global_Level_Items/Gems/Actors/Gem_Base_BP.Gem_Base_BP_C|GetGem_State _asgem_base_bp_3) "NewEnumerator2")) (not (Utilities|Enum|Equal(Enum) (Variables|/Game/SpyroContent/Global_Assets/Global_Level_Items/Gems/Actors/Gem_Base_BP.Gem_Base_BP_C|GetGem_State _asgem_base_bp_3) "NewEnumerator3")))
                    (CallFunction|LookforNearbyPlayer (Utilities|Array|MakeArray "ObjectTypeQuery9") _asgem_base_bp_3)))))
            (:then_1
              (Utilities|FlowControl|Delay 1.3)
              (if (Variables|Default|GetContainer_Destroyed)
                (bind _asgem_base_bp_4 (Utilities|Casting|CastToGem_Base_BP (Variables|/Script/Engine.ChildActorComponent|GetChildActor (Variables|Default|GetChildActor))))
                (Variables|/Game/SpyroContent/Global_Assets/Global_Level_Items/Gems/Actors/Gem_Base_BP.Gem_Base_BP_C|SetSparx_Cant_Grab_Me _asgem_base_bp_4 false)
                (Default|InvokedCheckifGemsNearGround _asgem_base_bp_4)))))))))

(event EventResetThisContainer
  (bind _asgem_base_bp (Utilities|Casting|CastToGem_Base_BP (Variables|/Script/Engine.ChildActorComponent|GetChildActor (Variables|Default|GetChildActor))))
  (if (not (Utilities|Enum|Equal(Enum) (Variables|/Game/SpyroContent/Global_Assets/Global_Level_Items/Gems/Actors/Gem_Base_BP.Gem_Base_BP_C|GetGem_State _asgem_base_bp) "NewEnumerator2"))
    (Variables|Default|SetGem%20is%20Springing false)
    (CallFunction|ToggleGemCollission false)
    (bind _asgem_base_bp_2 (Utilities|Casting|CastToGem_Base_BP (Variables|/Script/Engine.ChildActorComponent|GetChildActor (Variables|Default|GetChildActor)))
      (:then
        (Components|StaticMesh|SetStaticMesh (Variables|/Game/SpyroContent/Global_Assets/Global_Level_Items/Gems/Actors/Gem_Base_BP.Gem_Base_BP_C|GetVisual_Mesh _asgem_base_bp_2) "/Game/SpyroContent/Global_Assets/Global_Level_Items/Gems/Static_Meshes/gem_s1.gem_s1"))
      (:CastFailed
        _))
    (CallFunction|ManageGem'sFloatingAppearance (Variables|Default|GetChildActor) self)
    (Variables|/Game/SpyroContent/Global_Assets/Global_Level_Items/Gems/Actors/Gem_Base_BP.Gem_Base_BP_C|SetSparx_Cant_Grab_Me _asgem_base_bp true)
    (Rendering|SetVisibility (Variables|/Game/SpyroContent/Global_Assets/Global_Level_Items/Gems/Actors/Gem_Base_BP.Gem_Base_BP_C|GetDropshadow _asgem_base_bp) false false)
    (Components|Activation|Deactivate (Variables|Default|GetParticleSystem))
    (|CallParentFunction)
    (bind _childactor (Variables|Default|GetChildActor)
      (:then
        (Transformation|SetActorLocation (Variables|/Script/Engine.ChildActorComponent|GetChildActor _childactor) (Transformation|GetWorldLocation _childactor) false false))
      (:else))))

(fn ConstructionScript
  (|CallParentFunction))

(fn SetSpringChestMat
  (bind _staticmesh (Variables|Default|GetStaticMesh))
  (bind _asgem_base_bp (Utilities|Casting|CastToGem_Base_BP (Variables|/Script/Engine.ChildActorComponent|GetChildActor (Variables|Default|GetChildActor))))
  (bind _asspyro_save_data (CallFunction|LoadSpyroGame self))
  (Rendering|Material|SetMaterial _staticmesh 0 (Utilities|Select :Index (Variables|/Game/SpyroContent/Global_Assets/Global_Level_Items/Gems/Actors/Gem_Base_BP.Gem_Base_BP_C|GetValue _asgem_base_bp) :Option%200 "/Game/SpyroContent/Global_Assets/Global_Level_Items/Treasure_Containers/Spring_Chest/Materials/Spring_Chest_Red.Spring_Chest_Red" :Option%201 "/Game/SpyroContent/Global_Assets/Global_Level_Items/Treasure_Containers/Spring_Chest/Materials/Spring_Chest_Red.Spring_Chest_Red" :Option%202 "/Game/SpyroContent/Global_Assets/Global_Level_Items/Treasure_Containers/Spring_Chest/Materials/Spring_Chest_Green.Spring_Chest_Green" :Option%203 "/Game/SpyroContent/Global_Assets/Global_Level_Items/Treasure_Containers/Spring_Chest/Materials/Spring_Chest_Red.Spring_Chest_Red" :Option%204 "/Game/SpyroContent/Global_Assets/Global_Level_Items/Treasure_Containers/Spring_Chest/Materials/Spring_Chest_Red.Spring_Chest_Red" :Option%205 (select (Variables|/Game/SpyroContent/Global_Assets/Global_SaveData/Spyro_SaveData.Spyro_SaveData_C|GetS1_Treasure _asspyro_save_data) "/Game/SpyroContent/Global_Assets/Global_Level_Items/Treasure_Containers/Spring_Chest/Materials/Spring_Chest_Blue.Spring_Chest_Blue" "/Game/SpyroContent/Global_Assets/Global_Level_Items/Treasure_Containers/Spring_Chest/Materials/Spring_Chest_BlueishPurple.Spring_Chest_BlueishPurple") :Option%206 "/Game/SpyroContent/Global_Assets/Global_Level_Items/Treasure_Containers/Spring_Chest/Materials/Spring_Chest_Red.Spring_Chest_Red" :Option%207 "/Game/SpyroContent/Global_Assets/Global_Level_Items/Treasure_Containers/Spring_Chest/Materials/Spring_Chest_Red.Spring_Chest_Red" :Option%208 "/Game/SpyroContent/Global_Assets/Global_Level_Items/Treasure_Containers/Spring_Chest/Materials/Spring_Chest_Red.Spring_Chest_Red" :Option%209 "/Game/SpyroContent/Global_Assets/Global_Level_Items/Treasure_Containers/Spring_Chest/Materials/Spring_Chest_Red.Spring_Chest_Red" :Option%2010 (select (Variables|/Game/SpyroContent/Global_Assets/Global_SaveData/Spyro_SaveData.Spyro_SaveData_C|GetS1_Treasure _asspyro_save_data) "/Game/SpyroContent/Global_Assets/Global_Level_Items/Treasure_Containers/Spring_Chest/Materials/Spring_Chest_YellowS1.Spring_Chest_YellowS1" "/Game/SpyroContent/Global_Assets/Global_Level_Items/Treasure_Containers/Spring_Chest/Materials/Spring_Chest_Yellow.Spring_Chest_Yellow") :Option%2011 "/Game/SpyroContent/Global_Assets/Global_Level_Items/Treasure_Containers/Spring_Chest/Materials/Spring_Chest_Red.Spring_Chest_Red" :Option%2012 "/Game/SpyroContent/Global_Assets/Global_Level_Items/Treasure_Containers/Spring_Chest/Materials/Spring_Chest_Red.Spring_Chest_Red" :Option%2013 0 :Option%2014 0 :Option%2015 0 :Option%2016 0 :Option%2017 0 :Option%2018 0 :Option%2019 0 :Option%2020 0 :Option%2021 0 :Option%2022 0 :Option%2023 0 :Option%2024 0 :Option%2025 (select (Variables|/Game/SpyroContent/Global_Assets/Global_SaveData/Spyro_SaveData.Spyro_SaveData_C|GetS1_Treasure _asspyro_save_data) "/Game/SpyroContent/Global_Assets/Global_Level_Items/Treasure_Containers/Spring_Chest/Materials/Spring_Chest_Magenta_S1.Spring_Chest_Magenta_S1" "/Game/SpyroContent/Global_Assets/Global_Level_Items/Treasure_Containers/Spring_Chest/Materials/Spring_Chest_Magenta.Spring_Chest_Magenta")))
  (Rendering|Material|SetMaterial _staticmesh 2 (select (Variables|Default|GetGem%20is%20Springing) "/Game/SpyroContent/Global_Assets/Global_Materials/Material_Instances/Invisible_Mat.Invisible_Mat" (Utilities|Select :Index (Variables|/Game/SpyroContent/Global_Assets/Global_Level_Items/Gems/Actors/Gem_Base_BP.Gem_Base_BP_C|GetValue _asgem_base_bp) :Option%200 "/Game/SpyroContent/Global_Assets/Global_Level_Items/Treasure_Containers/Spring_Chest/Materials/Spring_Chest_Red.Spring_Chest_Red" :Option%201 "/Game/SpyroContent/Global_Assets/Global_Level_Items/Treasure_Containers/Spring_Chest/Materials/Spring_Chest_Red.Spring_Chest_Red" :Option%202 "/Game/SpyroContent/Global_Assets/Global_Level_Items/Treasure_Containers/Spring_Chest/Materials/Spring_Chest_Green.Spring_Chest_Green" :Option%203 "/Game/SpyroContent/Global_Assets/Global_Level_Items/Treasure_Containers/Spring_Chest/Materials/Spring_Chest_Red.Spring_Chest_Red" :Option%204 "/Game/SpyroContent/Global_Assets/Global_Level_Items/Treasure_Containers/Spring_Chest/Materials/Spring_Chest_Red.Spring_Chest_Red" :Option%205 (select (Variables|/Game/SpyroContent/Global_Assets/Global_SaveData/Spyro_SaveData.Spyro_SaveData_C|GetS1_Treasure _asspyro_save_data) "/Game/SpyroContent/Global_Assets/Global_Level_Items/Treasure_Containers/Spring_Chest/Materials/Spring_Chest_Blue.Spring_Chest_Blue" "/Game/SpyroContent/Global_Assets/Global_Level_Items/Treasure_Containers/Spring_Chest/Materials/Spring_Chest_BlueishPurple.Spring_Chest_BlueishPurple") :Option%206 "/Game/SpyroContent/Global_Assets/Global_Level_Items/Treasure_Containers/Spring_Chest/Materials/Spring_Chest_Red.Spring_Chest_Red" :Option%207 "/Game/SpyroContent/Global_Assets/Global_Level_Items/Treasure_Containers/Spring_Chest/Materials/Spring_Chest_Red.Spring_Chest_Red" :Option%208 "/Game/SpyroContent/Global_Assets/Global_Level_Items/Treasure_Containers/Spring_Chest/Materials/Spring_Chest_Red.Spring_Chest_Red" :Option%209 "/Game/SpyroContent/Global_Assets/Global_Level_Items/Treasure_Containers/Spring_Chest/Materials/Spring_Chest_Red.Spring_Chest_Red" :Option%2010 (select (Variables|/Game/SpyroContent/Global_Assets/Global_SaveData/Spyro_SaveData.Spyro_SaveData_C|GetS1_Treasure _asspyro_save_data) "/Game/SpyroContent/Global_Assets/Global_Level_Items/Treasure_Containers/Spring_Chest/Materials/Spring_Chest_YellowS1.Spring_Chest_YellowS1" "/Game/SpyroContent/Global_Assets/Global_Level_Items/Treasure_Containers/Spring_Chest/Materials/Spring_Chest_Yellow.Spring_Chest_Yellow") :Option%2011 "/Game/SpyroContent/Global_Assets/Global_Level_Items/Treasure_Containers/Spring_Chest/Materials/Spring_Chest_Red.Spring_Chest_Red" :Option%2012 "/Game/SpyroContent/Global_Assets/Global_Level_Items/Treasure_Containers/Spring_Chest/Materials/Spring_Chest_Red.Spring_Chest_Red" :Option%2013 0 :Option%2014 0 :Option%2015 0 :Option%2016 0 :Option%2017 0 :Option%2018 0 :Option%2019 0 :Option%2020 0 :Option%2021 0 :Option%2022 0 :Option%2023 0 :Option%2024 0 :Option%2025 (select (Variables|/Game/SpyroContent/Global_Assets/Global_SaveData/Spyro_SaveData.Spyro_SaveData_C|GetS1_Treasure _asspyro_save_data) "/Game/SpyroContent/Global_Assets/Global_Level_Items/Treasure_Containers/Spring_Chest/Materials/Spring_Chest_Magenta_S1.Spring_Chest_Magenta_S1" "/Game/SpyroContent/Global_Assets/Global_Level_Items/Treasure_Containers/Spring_Chest/Materials/Spring_Chest_Magenta.Spring_Chest_Magenta")))))

(fn LookforNearbyPlayer
  (params (ObjectTypes :type Array%20of%20EObjectTypeQuery%20Enums :default "ObjectTypeQuery1") (Gem%20Ref :type Gem%20Base%20BP%20Object%20Reference))
  (bind _childactor (Variables|Default|GetChildActor))
  (bind _childactor_2 (Variables|/Script/Engine.ChildActorComponent|GetChildActor _childactor))
  (bind _returnvalue (Transformation|GetActorLocation _childactor_2))
  (bind _asbp_base_playable (Utilities|Casting|CastToBP_Base_Playable (Variables|/Game/SpyroContent/Global_Assets/Global_Components/Damageable_Com.Damageable_Com_C|GetDeal%20Damage%20-%20Person%20Who%20Dealt%20the%20Damage (Variables|Default|GetDamageable))))
  (bind _outhits (Collision|MultiSphereTraceForObjects _returnvalue _returnvalue 286.0 ObjectTypes false 0 "None"))
  (bind _array_element (Utilities|Array|ForEachLoopwithBreak _outhits :!label _label)
    (:LoopBody
      (if (Math|Boolean|ANDBoolean (.bblockinghit _array_element) (== (.hitactor _array_element) _asbp_base_playable) (== (.hitcomponent _array_element) (Variables|/Script/Engine.Character|GetCapsuleComponent _asbp_base_playable)))
        (Variables|/Game/SpyroContent/Global_Assets/Global_Level_Items/Gems/Actors/Gem_Base_BP.Gem_Base_BP_C|SetSparx_Cant_Grab_Me Gem%20Ref false)
        (Default|ChangeGemState Gem%20Ref "NewEnumerator3" _asbp_base_playable)
        (goto _label Break)))))

(fn ToggleGemCollission
  (params (On/Off :type Boolean))
  (bind _returnvalue (select On/Off "ECR_Overlap" "ECR_Ignore"))
  (bind _asgem_base_bp (Utilities|Casting|CastToGem_Base_BP (Variables|/Script/Engine.ChildActorComponent|GetChildActor (Variables|Default|GetChildActor))))
  (Utilities|IsValid _asgem_base_bp
    (:Is%20Valid
      (Collision|SetCollisionResponsetoChannel (Variables|/Game/SpyroContent/Global_Assets/Global_Level_Items/Gems/Actors/Gem_Base_BP.Gem_Base_BP_C|GetCollection_Radius _asgem_base_bp) "ECC_Pawn" _returnvalue)
      (Collision|SetCollisionResponsetoChannel (Variables|/Game/SpyroContent/Global_Assets/Global_Level_Items/Gems/Actors/Gem_Base_BP.Gem_Base_BP_C|GetCollection_Radius _asgem_base_bp) "ECC_GameTraceChannel4" _returnvalue)
      (Collision|SetCollisionResponsetoChannel (Variables|/Game/SpyroContent/Global_Assets/Global_Level_Items/Gems/Actors/Gem_Base_BP.Gem_Base_BP_C|GetCollection_Radius _asgem_base_bp) "ECC_GameTraceChannel2" _returnvalue)
      (Collision|SetCollisionResponsetoChannel (Variables|/Game/SpyroContent/Global_Assets/Global_Level_Items/Gems/Actors/Gem_Base_BP.Gem_Base_BP_C|GetCollection_Radius _asgem_base_bp) "ECC_GameTraceChannel5" _returnvalue))))

(event Custom|Gem%20Spring
  (bind _returnvalue (Transformation|GetActorLocation))
  (bind _returnvalue_2 (Transformation|GetActorLocation))
  (bind _newtrack_0 (Timeline|Timeline_3 PlayFromStart)
    (:Update
      (bind _childactor (Variables|Default|GetChildActor)
        (:then
          (Utilities|IsValid (Variables|/Script/Engine.ChildActorComponent|GetChildActor _childactor)
            (:Is%20Valid
              (Transformation|SetWorldLocation (Variables|/Script/Engine.Actor|GetRootComponent (Variables|/Script/Engine.ChildActorComponent|GetChildActor _childactor)) (Math|Vector|MakeVector (+ (.x _returnvalue_2) 2.0) (.y _returnvalue_2) (+ (.z _returnvalue_2) (Math|Float|Lerp 64.0 224.0 _newtrack_0))) false false))))
        (:else)))
    (:Finished
      (bind _childactor_2 (Variables|Default|GetChildActor)
        (:then
          (Transformation|SetWorldLocation (Variables|/Script/Engine.Actor|GetRootComponent (Variables|/Script/Engine.ChildActorComponent|GetChildActor _childactor_2)) (Math|Vector|MakeVector (.x _returnvalue) (.y _returnvalue) (+ (.z _returnvalue) 24.0)) false false)
          (Timeline|Timeline_3 Stop))
        (:else)))))