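; Fire Container is a treasure container that damages a playable character whose capsule hits or overlaps it, unless that character is in one exempt state.
; It accepts only six specific damage types, and only while intact and not invincible.
; An accepted hit reports success to its Damageable component and spawns wafting smoke at the container's scale.
; It extends the parent's damage and reset handling to stop its audio and replay it on reset if not destroyed.
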(event OnComponentHit(CapsuleComponent)
  (params (HitComponent :type Primitive%20Component%20Object%20Reference) (OtherActor :type Actor%20Object%20Reference) (OtherComp :type Primitive%20Component%20Object%20Reference) (NormalImpulse :type Vector :default "0, 0, 0") (Hit :type Hit%20Result%20Structure%20%28by%20ref%29))
  (CallFunction|Damage? OtherActor OtherComp))

(event OnComponentBeginOverlap(CapsuleComponent)
  (params (OverlappedComponent :type Primitive%20Component%20Object%20Reference) (OtherActor :type Actor%20Object%20Reference) (OtherComp :type Primitive%20Component%20Object%20Reference) (OtherBodyIndex :type Integer) (bFromSweep :type Boolean) (SweepResult :type Hit%20Result%20Structure%20%28by%20ref%29))
  (CallFunction|Damage? OtherActor OtherComp))

(event EventTreasureContainerSuccessfullyDamaged
  (|CallParentFunction)
  (Audio|Components|Audio|Stop (Variables|Default|GetAudio)))

(event EventResetThisContainer
  (|CallParentFunction)
  (if (not (Variables|Default|GetContainer_Destroyed))
    (Audio|Components|Audio|Play (Variables|Default|GetAudio) 0.0)))

(event EventDealDamagetoTreasureContainer
  (bind _damageable (Variables|Default|GetDamageable))
  (bind _deal_damage___damage_type (Variables|/Game/SpyroContent/Global_Assets/Global_Components/Damageable_Com.Damageable_Com_C|GetDeal%20Damage%20-%20Damage%20Type _damageable))
  (if (Math|Boolean|ANDBoolean (not (Variables|Default|GetContainer_Destroyed)) (not (Variables|/Game/SpyroContent/Global_Assets/Global_Components/Damageable_Com.Damageable_Com_C|GetInvincible _damageable)) (Math|Boolean|ORBoolean (Utilities|Enum|Equal(Enum) _deal_damage___damage_type "NewEnumerator7") (Utilities|Enum|Equal(Enum) _deal_damage___damage_type "NewEnumerator9") (Utilities|Enum|Equal(Enum) _deal_damage___damage_type "NewEnumerator10") (Utilities|Enum|Equal(Enum) _deal_damage___damage_type "NewEnumerator11") (Utilities|Enum|Equal(Enum) _deal_damage___damage_type "NewEnumerator12") (Utilities|Enum|Equal(Enum) _deal_damage___damage_type "NewEnumerator13")))
    (Default|CallDamageWasSuccessfullyDealt (Variables|Default|GetDamageable))
    (Effects|SpawnEmitteratLocation "/Game/SpyroContent/Global_Assets/Global_Level_Items/Dragon_Breath/Particles/smoke_wafting.smoke_wafting" (Transformation|GetActorLocation) "0, 0, 0" (Transformation|GetActorScale3D))))

(fn ConstructionScript
  (|CallParentFunction))

(fn Damage?
  (params (Object :type Object%20Object%20Reference) (B :type Object%20Object%20Reference))
  (bind _asbp_base_playable (Utilities|Casting|CastToBP_Base_Playable Object))
  (if (and (== (Variables|/Script/Engine.Character|GetCapsuleComponent _asbp_base_playable) B) (not (Utilities|Enum|Equal(Enum) (Variables|/Game/SpyroContent/Global_Assets/Global_Characters/Playable_Characters/BP_Base_Playable.BP_Base_Playable_C|GetPlayer_State _asbp_base_playable) "NewEnumerator19")))
    (Default|DealDamage (Variables|/Game/SpyroContent/Global_Assets/Global_Characters/Playable_Characters/BP_Base_Playable.BP_Base_Playable_C|GetDamageable _asbp_base_playable) "NewEnumerator1" "0, 0, 0" false 0 false)))