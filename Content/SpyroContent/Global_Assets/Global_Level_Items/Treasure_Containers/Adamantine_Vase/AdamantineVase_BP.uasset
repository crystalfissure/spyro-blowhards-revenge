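; Adamantine Vase is a treasure container Blueprint that only registers damage from one specific damage type when it is a super attack.
; On BeginPlay it runs the parent logic, marks its static mesh as the metal material component on the Damageable component, and binds to damage events.
; The damage handler confirms a successful hit only while the container is intact and both conditions are met.
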(event Custom|On%20Damage%20Dealt
  (bind _damageable (Variables|Default|GetDamageable))
  (if (Math|Boolean|ANDBoolean (not (Variables|Default|GetContainer_Destroyed)) (Utilities|Enum|Equal(Enum) (Variables|/Game/SpyroContent/Global_Assets/Global_Components/Damageable_Com.Damageable_Com_C|GetDeal%20Damage%20-%20Damage%20Type _damageable) "NewEnumerator4") (Variables|/Game/SpyroContent/Global_Assets/Global_Components/Damageable_Com.Damageable_Com_C|GetDeal%20Damage%20-%20Super%20Damage _damageable))
    (Default|CallDamageWasSuccessfullyDealt (Variables|Default|GetDamageable))))

(event EventBeginPlay
  (|CallParentFunction)
  (Variables|/Game/SpyroContent/Global_Assets/Global_Components/Damageable_Com.Damageable_Com_C|SetComponent_with_Metal_Material (Variables|Default|GetDamageable) (Variables|Default|GetStaticMesh))
  (EventDispatchers|BindEventtoCallDealDamage (Variables|Default|GetDamageable) (delegate Custom|On%20Damage%20Dealt)))

(fn ConstructionScript
  (|CallParentFunction))