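; Exploding bottle treasure container that, depending on incoming damage type, explodes at once, lights a wobbling timed fuse, or has its lit fuse put out.
; Exploding launches it spinning upward, spawns shards and smoke, then reports successful damage when the flight ends.
; A sphere trace deals super damage to nearby Damageable hitboxes, with other bottles delayed briefly for chain reactions.
; Resetting the container restores the mesh, fuse, countdown, launch and stored damage data.
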(event Custom|On%20Damage%20Attempted
  (bind _damageable (Variables|Default|GetDamageable))
  (bind _deal_damage___damage_type (Variables|/Game/SpyroContent/Global_Assets/Global_Components/Damageable_Com.Damageable_Com_C|GetDeal%20Damage%20-%20Damage%20Type _damageable))
  (Utilities|FlowControl|Delay 0.1)
  (if (not (Variables|Default|GetContainer_Destroyed))
    (if (Math|Boolean|ORBoolean (Utilities|Enum|Equal(Enum) _deal_damage___damage_type "NewEnumerator4") (Utilities|Enum|Equal(Enum) _deal_damage___damage_type "NewEnumerator2") (Utilities|Enum|Equal(Enum) _deal_damage___damage_type "NewEnumerator8") (Utilities|Enum|Equal(Enum) _deal_damage___damage_type "NewEnumerator0") (Variables|/Game/SpyroContent/Global_Assets/Global_Components/Damageable_Com.Damageable_Com_C|GetDeal%20Damage%20-%20Super%20Damage _damageable))
      (CallFunction|Explode)
      (elif (Math|Boolean|ANDBoolean (or (Utilities|Enum|Equal(Enum) _deal_damage___damage_type "NewEnumerator1") (Utilities|Enum|Equal(Enum) _deal_damage___damage_type "NewEnumerator3")) (not (Variables|Default|GetFuse_Lit)) (not (Variables|Default|GetExploded)))
        (Variables|Default|SetFuse_Lit true)
        (CallFunction|FuseLitWobble)
        (Components|Activation|Activate (Variables|Default|GetParticle1) false)
        (bind _returnvalue (Utilities|Time|SetTimerbyFunctionName 0 "Explosion Countdown" 1.0 true))
        (Variables|Default|SetCountdown%20Timer _returnvalue)
        (elif (Math|Boolean|ANDBoolean (Math|Boolean|ORBoolean (Utilities|Enum|Equal(Enum) _deal_damage___damage_type "NewEnumerator13") (Utilities|Enum|Equal(Enum) _deal_damage___damage_type "NewEnumerator10") (Utilities|Enum|Equal(Enum) _deal_damage___damage_type "NewEnumerator11") (Utilities|Enum|Equal(Enum) _deal_damage___damage_type "NewEnumerator9") (Utilities|Enum|Equal(Enum) _deal_damage___damage_type "NewEnumerator7")) (Variables|Default|GetFuse_Lit) (not (Variables|Default|GetExploded)))
          (Variables|Default|SetFuse_Lit false)
          (Components|Activation|Deactivate (Variables|Default|GetParticle1))
          (Utilities|Time|ClearandInvalidateTimerbyHandle (Variables|Default|GetCountdown%20Timer))
          (Variables|Default|SetCountdown_to_Explosion 2))))))

(event Custom|Fuse%20Lit%20Wobble
  (bind _newtrack_0 (Timeline|Timeline_3 PlayFromStart)
    (:Update
      (Transformation|SetRelativeRotation (Variables|Default|GetStaticMesh) (Math|Rotator|MakeRotator 0.0 _newtrack_0 0.0) false false))
    (:Finished
      (if (and (Variables|Default|GetFuse_Lit) (not (Variables|Default|GetExploded)))
        (CallFunction|FuseLitWobble)))))

(event Custom|Launch%20Bottle
  (bind _damageable (Variables|Default|GetDamageable))
  (bind _newtrack_0 (Timeline|Timeline_4 PlayFromStart)
    (:Update
      (Transformation|SetRelativeLocationAndRotation (Variables|Default|GetCapsule%20Component) (Math|Vector|MakeVector 0.0 0.0 (Math|Float|Lerp 41.0 6e+02 _newtrack_0)) (Math|Rotator|MakeRotator (- (.roll (Transformation|GetWorldRotation (Variables|Default|GetCapsule%20Component))) (* (Utilities|Time|GetWorldDeltaSeconds) 4e+02)) 0.0 0.0) false false))
    (:Finished
      (if (not (Variables|Default|GetContainer_Destroyed))
        (Variables|/Game/SpyroContent/Global_Assets/Global_Components/Damageable_Com.Damageable_Com_C|SetDeal%20Damage%20-%20Damage%20Type _damageable "NewEnumerator0")
        (Variables|/Game/SpyroContent/Global_Assets/Global_Components/Damageable_Com.Damageable_Com_C|SetDeal%20Damage%20-%20Magnetize%20Immediately _damageable false)
        (Default|CallDamageWasSuccessfullyDealt _damageable)
        (Transformation|SetRelativeLocationAndRotation (Variables|Default|GetCapsule%20Component) "0, 0,41.000000" "0, 0, 0" false false)))))

(event Custom|Stop%20Bottle%20Launch
  (bind _damageable (Variables|Default|GetDamageable))
  (Utilities|FlowControl|Sequence
    (:then_0
      (bind _newtrack_0 (Timeline|Timeline_4 Stop)
        (:Update
          (Transformation|SetRelativeLocationAndRotation (Variables|Default|GetCapsule%20Component) (Math|Vector|MakeVector 0.0 0.0 (Math|Float|Lerp 41.0 6e+02 _newtrack_0)) (Math|Rotator|MakeRotator (- (.roll (Transformation|GetWorldRotation (Variables|Default|GetCapsule%20Component))) (* (Utilities|Time|GetWorldDeltaSeconds) 4e+02)) 0.0 0.0) false false))
        (:Finished
          (if (not (Variables|Default|GetContainer_Destroyed))
            (Variables|/Game/SpyroContent/Global_Assets/Global_Components/Damageable_Com.Damageable_Com_C|SetDeal%20Damage%20-%20Damage%20Type _damageable "NewEnumerator0")
            (Variables|/Game/SpyroContent/Global_Assets/Global_Components/Damageable_Com.Damageable_Com_C|SetDeal%20Damage%20-%20Magnetize%20Immediately _damageable false)
            (Default|CallDamageWasSuccessfullyDealt _damageable)
            (Transformation|SetRelativeLocationAndRotation (Variables|Default|GetCapsule%20Component) "0, 0,41.000000" "0, 0, 0" false false :!label _label)))))
    (:then_1
      (goto _label))))

(event Custom|Explode
  (bind _capsule_component (Variables|Default|GetCapsule%20Component))
  (bind _returnvalue (Transformation|GetWorldLocation _capsule_component))
  (if (not (Variables|Default|GetExploded))
    (Utilities|Time|ClearandInvalidateTimerbyHandle (Variables|Default|GetCountdown%20Timer))
    (Variables|Default|SetExploded true)
    (Variables|Default|SetFuse_Lit false)
    (CallFunction|LaunchBottle)
    (Components|Activation|Deactivate (Variables|Default|GetParticle1))
    (bind _returnvalue_2 (Game|SpawnActorfromClass "/Game/SpyroContent/Global_Assets/Global_Level_Items/Treasure_Containers/Basket/Actors/Basket_Burst_BP.Basket_Burst_BP_C" (Transformation|GetActorTransform) "AlwaysSpawn" 0 0))
    (Default|ShardBurstAction _returnvalue_2 "/Game/SpyroContent/Global_Assets/Global_Level_Items/Treasure_Containers/Exploding_Bottle/exploding_bottle_shard_1.exploding_bottle_shard_1")
    (Audio|PlaySoundatLocation "/Game/SpyroContent/Global_Assets/Global_Level_Items/Treasure_Containers/Vase/vase_shatter.vase_shatter" (Transformation|GetActorLocation) "0, 0, 0" 1.0 1.0 0.0 0 0 0)
    (Default|ActivateBlackSmoke _returnvalue_2)
    (Components|StaticMesh|SetStaticMesh (Variables|Default|GetStaticMesh) "/Game/SpyroContent/Global_Assets/Global_Level_Items/Treasure_Containers/Exploding_Bottle/exploding_bottle_exploded.exploding_bottle_exploded")
    (bind _outhits (Collision|MultiSphereTraceForObjects _returnvalue _returnvalue 2e+02 (Utilities|Array|MakeArray "ObjectTypeQuery1" "ObjectTypeQuery2" "ObjectTypeQuery3" "ObjectTypeQuery4" "ObjectTypeQuery8" "ObjectTypeQuery9" "ObjectTypeQuery10") false 0 "None"))
    (for _array_element _outhits
      (Utilities|IsValid (.hitactor _array_element)
        (:Is%20Valid
          (Utilities|IsValid (Actor|GetComponentbyClass (.hitactor _array_element) "/Game/SpyroContent/Global_Assets/Global_Components/Damageable_Com.Damageable_Com_C")
            (:Is%20Valid
              (if (and (.bblockinghit _array_element) (== (Variables|/Game/SpyroContent/Global_Assets/Global_Components/Damageable_Com.Damageable_Com_C|GetObject's%20Hitbox%20Component (Actor|GetComponentbyClass (.hitactor _array_element) "/Game/SpyroContent/Global_Assets/Global_Components/Damageable_Com.Damageable_Com_C")) (.hitcomponent _array_element)))
                (bind _asexploding_bottle_bp (Utilities|Casting|CastToExplodingBottle_BP (.hitactor _array_element))
                  (:then
                    (CallFunction|DelayedBreakOtherBottle _asexploding_bottle_bp))
                  (:CastFailed
                    (CallFunction|DealExplosionDamage (.hitcomponent _array_element) (Actor|GetComponentbyClass (.hitactor _array_element) "/Game/SpyroContent/Global_Assets/Global_Components/Damageable_Com.Damageable_Com_C"))))))))))))

(event Custom|Delayed%20Break%20Other%20Bottle
  (Utilities|FlowControl|Delay 0.2)
  (CallFunction|DealExplosionDamage (Variables|Default|GetCapsule%20Component) (Variables|Default|GetDamageable)))

(event EventResetThisContainer
  (bind _damageable (Variables|Default|GetDamageable))
  (|CallParentFunction)
  (Components|StaticMesh|SetStaticMesh (Variables|Default|GetStaticMesh) "/Game/SpyroContent/Global_Assets/Global_Level_Items/Treasure_Containers/Exploding_Bottle/exploding_bottle.exploding_bottle")
  (Variables|Default|SetExploded false)
  (Components|Activation|Deactivate (Variables|Default|GetParticle1))
  (Utilities|Time|ClearandInvalidateTimerbyHandle (Variables|Default|GetCountdown%20Timer))
  (Variables|Default|SetCountdown_to_Explosion 2)
  (Variables|Default|SetFuse_Lit false)
  (CallFunction|StopBottleLaunch)
  (Variables|/Game/SpyroContent/Global_Assets/Global_Components/Damageable_Com.Damageable_Com_C|SetDeal%20Damage%20-%20Attackers%20Forward%20Vector _damageable "0, 0, 0")
  (Variables|/Game/SpyroContent/Global_Assets/Global_Components/Damageable_Com.Damageable_Com_C|SetDeal%20Damage%20-%20Damage%20Type _damageable "NewEnumerator6")
  (Variables|/Game/SpyroContent/Global_Assets/Global_Components/Damageable_Com.Damageable_Com_C|SetDeal%20Damage%20-%20Magnetize%20Immediately _damageable false)
  (Variables|/Game/SpyroContent/Global_Assets/Global_Components/Damageable_Com.Damageable_Com_C|SetDeal%20Damage%20-%20Person%20Who%20Dealt%20the%20Damage _damageable 0)
  (Variables|/Game/SpyroContent/Global_Assets/Global_Components/Damageable_Com.Damageable_Com_C|SetDeal%20Damage%20-%20Super%20Damage _damageable false))

(event EventBeginPlay
  (|CallParentFunction)
  (EventDispatchers|BindEventtoDamageWasAttempted (Variables|Default|GetDamageable) (delegate Custom|On%20Damage%20Attempted)))

(fn ConstructionScript
  (|CallParentFunction))

(fn ExplosionCountdown
  (bind _output_get (Variables|Default|SetCountdown_to_Explosion (select (<= (- (Variables|Default|GetCountdown_to_Explosion) 1) 0) 0 (- (Variables|Default|GetCountdown_to_Explosion) 1))))
  (if (<= _output_get 0)
    (CallFunction|Explode)))

(fn DealExplosionDamage
  (params (Hit%20Comp :type Scene%20Component%20Object%20Reference) (Damageable%20Comp :type Damageable%20Com%20Object%20Reference))
  (bind _returnvalue (Transformation|GetWorldLocation Hit%20Comp))
  (bind _returnvalue_2 (Transformation|GetActorLocation))
  (bind _returnvalue_3 (Math|Rotator|FindLookatRotation _returnvalue_2 _returnvalue))
  (bind _returnvalue_4 (Math|Vector|GetForwardVector _returnvalue_3))
  (Variables|/Game/SpyroContent/Global_Assets/Global_Components/Damageable_Com.Damageable_Com_C|SetDeal%20Damage%20-%20Attackers%20Forward%20Vector Damageable%20Comp _returnvalue_4)
  (Variables|/Game/SpyroContent/Global_Assets/Global_Components/Damageable_Com.Damageable_Com_C|SetDeal%20Damage%20-%20Damage%20Type Damageable%20Comp "NewEnumerator4")
  (Variables|/Game/SpyroContent/Global_Assets/Global_Components/Damageable_Com.Damageable_Com_C|SetDeal%20Damage%20-%20Magnetize%20Immediately Damageable%20Comp false)
  (Variables|/Game/SpyroContent/Global_Assets/Global_Components/Damageable_Com.Damageable_Com_C|SetDeal%20Damage%20-%20Person%20Who%20Dealt%20the%20Damage Damageable%20Comp 0)
  (Variables|/Game/SpyroContent/Global_Assets/Global_Components/Damageable_Com.Damageable_Com_C|SetDeal%20Damage%20-%20Super%20Damage Damageable%20Comp true)
  (Default|DealDamage Damageable%20Comp "NewEnumerator4" _returnvalue_4 true 0 false))