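; Propeller chest treasure container that hovers in the air, bobbing up and down around its starting height.
; Two timelines alternately lerp the actor's Z and restart each other when finished, creating an endless float loop.
; On BeginPlay a downward line trace pins the drop shadow just above the ground in absolute space.
; Its audio stops when successfully damaged and replays on reset if the container is not destroyed.
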(event Custom|Chest%20Float%20Down
  (bind _returnvalue (Transformation|GetActorLocation))
  (bind _returnvalue_2 (Math|Float|MakeLiteralFloat 2e+01))
  (bind _returnvalue_3 (Transformation|GetActorLocation))
  (bind _starting_z_loc (Variables|Default|GetStarting_Z_Loc))
  (bind _starting_z_loc_2 (Variables|Default|GetStarting_Z_Loc))
  (Utilities|FlowControl|Sequence
    (:then_0
      (bind _newtrack_0 (Timeline|Timeline_3 Stop)
        (:Update
          (Transformation|SetActorLocation (Math|Vector|MakeVector (.x _returnvalue) (.y _returnvalue) (Math|Float|Lerp (- _starting_z_loc_2 _returnvalue_2) (+ _starting_z_loc_2 _returnvalue_2) _newtrack_0)) false false))
        (:Finished
          (CallFunction|ChestFloatDown))))
    (:then_1
      (bind _newtrack_0_2 (Timeline|Timeline_4 PlayFromStart)
        (:Update
          (Transformation|SetActorLocation (Math|Vector|MakeVector (.x _returnvalue_3) (.y _returnvalue_3) (Math|Float|Lerp (+ _starting_z_loc _returnvalue_2) (- _starting_z_loc _returnvalue_2) _newtrack_0_2)) false false))
        (:Finished
          (CallFunction|ChestFloatUp))))))

(event Custom|Chest%20Float%20Up
  (bind _returnvalue (Transformation|GetActorLocation))
  (bind _returnvalue_2 (Math|Float|MakeLiteralFloat 2e+01))
  (bind _returnvalue_3 (Transformation|GetActorLocation))
  (bind _starting_z_loc (Variables|Default|GetStarting_Z_Loc))
  (bind _starting_z_loc_2 (Variables|Default|GetStarting_Z_Loc))
  (Utilities|FlowControl|Sequence
    (:then_0
      (bind _newtrack_0 (Timeline|Timeline_4 Stop)
        (:Update
          (Transformation|SetActorLocation (Math|Vector|MakeVector (.x _returnvalue_3) (.y _returnvalue_3) (Math|Float|Lerp (+ _starting_z_loc _returnvalue_2) (- _starting_z_loc _returnvalue_2) _newtrack_0)) false false))
        (:Finished
          (CallFunction|ChestFloatUp))))
    (:then_1
      (bind _newtrack_0_2 (Timeline|Timeline_3 PlayFromStart)
        (:Update
          (Transformation|SetActorLocation (Math|Vector|MakeVector (.x _returnvalue) (.y _returnvalue) (Math|Float|Lerp (- _starting_z_loc_2 _returnvalue_2) (+ _starting_z_loc_2 _returnvalue_2) _newtrack_0_2)) false false))
        (:Finished
          (CallFunction|ChestFloatDown))))))

(event EventBeginPlay
  (bind _returnvalue (Transformation|GetActorLocation))
  (bind _dropshadow (Variables|Default|GetDropshadow))
  (bind (_x _y _z) (Math|Vector|BreakVector _returnvalue))
  (|CallParentFunction)
  (Variables|Default|SetStarting_Z_Loc (.z (Transformation|GetActorLocation)))
  (CallFunction|ChestFloatUp)
  (bind _outhit (Collision|LineTraceForObjects _returnvalue (Math|Vector|MakeVector _x _y (- _z 1e+04)) (Utilities|Array|MakeArray "ObjectTypeQuery1") false 0 "None"))
  (if (.bblockinghit _outhit)
    (Variables|/Script/Engine.SceneComponent|SetbAbsoluteLocation _dropshadow true)
    (Transformation|SetWorldLocation _dropshadow (Math|Vector|MakeVector (.X (Math|Vector|BreakVector (.location _outhit))) (.Y (Math|Vector|BreakVector (.location _outhit))) (+ (.Z (Math|Vector|BreakVector (.location _outhit))) 3.0)) false false)))

(event EventTreasureContainerSuccessfullyDamaged
  (|CallParentFunction)
  (Audio|Components|Audio|Stop (Variables|Default|GetAudio)))

(event EventResetThisContainer
  (|CallParentFunction)
  (if (not (Variables|Default|GetContainer_Destroyed))
    (Audio|Components|Audio|Play (Variables|Default|GetAudio) 0.0)))

(fn ConstructionScript
  (|CallParentFunction))