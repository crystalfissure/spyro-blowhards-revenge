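; Adamantine chest treasure container that resists damage until struck by one specific damage type flagged as super damage.
; Binds to its Damageable component on BeginPlay and reports successful damage only for that qualifying hit while the container is intact.
; Resisted attempts play a strong bump sound at the chest, skipped in S1Mode and throttled by a DoOnce that resets after a short delay.
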(event Custom|When%20Damage%20is%20Attempted
  (Utilities|FlowControl|DoOnce false :!label _label
    (:Completed
      (if (Variables|Default|GetS1_Mode)
        _
        (else
          (Audio|PlaySoundatLocation "/Game/SpyroContent/Global_Assets/Global_Level_Items/Treasure_Containers/Strong_Chest/strong_chest_bump.strong_chest_bump" (Transformation|GetActorLocation) "0, 0, 0" 1.0 1.0 0.0 0 0 0)))
      (Utilities|FlowControl|Delay 1.0)
      (goto _label Reset))))

(event Custom|On%20Damage%20Dealt
  (bind _damageable (Variables|Default|GetDamageable))
  (if (Math|Boolean|ANDBoolean (not (Variables|Default|GetContainer_Destroyed)) (Utilities|Enum|Equal(Enum) (Variables|/Game/SpyroContent/Global_Assets/Global_Components/Damageable_Com.Damageable_Com_C|GetDeal%20Damage%20-%20Damage%20Type _damageable) "NewEnumerator4") (Variables|/Game/SpyroContent/Global_Assets/Global_Components/Damageable_Com.Damageable_Com_C|GetDeal%20Damage%20-%20Super%20Damage _damageable))
    (Default|CallDamageWasSuccessfullyDealt (Variables|Default|GetDamageable))))

(event EventBeginPlay
  (|CallParentFunction)
  (EventDispatchers|BindEventtoDamageWasAttemptedButI'mResistant (Variables|Default|GetDamageable) (delegate Custom|When%20Damage%20is%20Attempted))
  (EventDispatchers|BindEventtoCallDealDamage (Variables|Default|GetDamageable) (delegate Custom|On%20Damage%20Dealt)))

(fn ConstructionScript
  (|CallParentFunction))