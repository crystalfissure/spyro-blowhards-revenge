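; Treasure container vase hanging from a balloon, which bobs in place until a hit pops the balloon and drops it to break and release its item.
; Two alternating timelines drive the bob, and a downward trace places the drop shadow.
; On pop, another trace finds the floor and Tick lowers the vase, then re-applies damage on landing to trigger the parent's destruction.
; Container reset restores height, materials, hitbox and item-drop lock.
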(event Custom|Balloon%20Float%20Down
  (bind _returnvalue (Transformation|GetActorLocation))
  (bind _returnvalue_2 (Math|Float|MakeLiteralFloat 2e+01))
  (bind _returnvalue_3 (Transformation|GetActorLocation))
  (bind _starting_z_loc (Variables|Default|GetStarting_Z_Loc))
  (bind _starting_z_loc_2 (Variables|Default|GetStarting_Z_Loc))
  (Utilities|FlowControl|Sequence
    (:then_0
      (bind _newtrack_0 (Timeline|Timeline_2_0 Stop)
        (:Update
          (if (Variables|Default|GetBalloon_Popped)
            (Timeline|Timeline_2_0 Stop)
            (else
              (Transformation|SetActorLocation (Math|Vector|MakeVector (.x _returnvalue) (.y _returnvalue) (Math|Float|Lerp (- _starting_z_loc_2 _returnvalue_2) (+ _starting_z_loc_2 _returnvalue_2) _newtrack_0)) false false))))
        (:Finished
          (if (not (Variables|Default|GetBalloon_Popped))
            (CallFunction|BalloonFloatDown)))))
    (:then_1
      (bind _newtrack_0_2 (Timeline|Timeline_3 PlayFromStart)
        (:Update
          (if (Variables|Default|GetBalloon_Popped)
            (Timeline|Timeline_3 Stop)
            (else
              (Transformation|SetActorLocation (Math|Vector|MakeVector (.x _returnvalue_3) (.y _returnvalue_3) (Math|Float|Lerp (+ _starting_z_loc _returnvalue_2) (- _starting_z_loc _returnvalue_2) _newtrack_0_2)) false false))))
        (:Finished
          (if (not (Variables|Default|GetBalloon_Popped))
            (CallFunction|BalloonFloatUp)))))))

(event Custom|Balloon%20Float%20Up
  (bind _returnvalue (Transformation|GetActorLocation))
  (bind _returnvalue_2 (Math|Float|MakeLiteralFloat 2e+01))
  (bind _returnvalue_3 (Transformation|GetActorLocation))
  (bind _starting_z_loc (Variables|Default|GetStarting_Z_Loc))
  (bind _starting_z_loc_2 (Variables|Default|GetStarting_Z_Loc))
  (Utilities|FlowControl|Sequence
    (:then_0
      (bind _newtrack_0 (Timeline|Timeline_3 Stop)
        (:Update
          (if (Variables|Default|GetBalloon_Popped)
            (Timeline|Timeline_3 Stop)
            (else
              (Transformation|SetActorLocation (Math|Vector|MakeVector (.x _returnvalue_3) (.y _returnvalue_3) (Math|Float|Lerp (+ _starting_z_loc _returnvalue_2) (- _starting_z_loc _returnvalue_2) _newtrack_0)) false false))))
        (:Finished
          (if (not (Variables|Default|GetBalloon_Popped))
            (CallFunction|BalloonFloatUp)))))
    (:then_1
      (bind _newtrack_0_2 (Timeline|Timeline_2_0 PlayFromStart)
        (:Update
          (if (Variables|Default|GetBalloon_Popped)
            (Timeline|Timeline_2_0 Stop)
            (else
              (Transformation|SetActorLocation (Math|Vector|MakeVector (.x _returnvalue) (.y _returnvalue) (Math|Float|Lerp (- _starting_z_loc_2 _returnvalue_2) (+ _starting_z_loc_2 _returnvalue_2) _newtrack_0_2)) false false))))
        (:Finished
          (if (not (Variables|Default|GetBalloon_Popped))
            (CallFunction|BalloonFloatDown)))))))

(event Custom|Reset%20On%20Damaged
  (bind _returnvalue (Transformation|GetActorLocation))
  (bind _staticmesh (Variables|Default|GetStaticMesh))
  (bind _balloon_hitbox (Variables|Default|GetBalloon_Hitbox))
  (bind (_x _y _z) (Math|Vector|BreakVector _returnvalue))
  (bind _returnvalue_2 (Transformation|GetWorldLocation _balloon_hitbox))
  (Utilities|FlowControl|DoOnce false) ; enters at Reset
)

(event Custom|Reset%20On%20Vase%20Hits%20Floor
  (bind _returnvalue (Transformation|GetActorLocation))
  (Utilities|FlowControl|DoOnce false) ; enters at Reset
)

(event EventBeginPlay
  (bind _returnvalue (Transformation|GetActorLocation))
  (bind _dropshadow (Variables|Default|GetDropshadow))
  (bind (_x _y _z) (Math|Vector|BreakVector _returnvalue))
  (|CallParentFunction)
  (Variables|/Game/SpyroContent/Global_Assets/Global_Components/Damageable_Com.Damageable_Com_C|SetObject's%20Hitbox%20Component (Variables|Default|GetDamageable) (Variables|Default|GetBalloon_Hitbox))
  (Variables|Default|SetStarting_Z_Loc (.z (Transformation|GetActorLocation)))
  (CallFunction|BalloonFloatUp)
  (bind _outhit (Collision|LineTraceForObjects _returnvalue (Math|Vector|MakeVector _x _y (- _z 1e+04)) (Utilities|Array|MakeArray "ObjectTypeQuery1") false 0 "None"))
  (if (.bblockinghit _outhit)
    (Variables|/Script/Engine.SceneComponent|SetbAbsoluteLocation _dropshadow true)
    (Transformation|SetWorldLocation _dropshadow (Math|Vector|MakeVector (.X (Math|Vector|BreakVector (.location _outhit))) (.Y (Math|Vector|BreakVector (.location _outhit))) (+ (.Z (Math|Vector|BreakVector (.location _outhit))) 3.0)) false false)))

(event EventTreasureContainerSuccessfullyDamaged
  (bind _returnvalue (Transformation|GetActorLocation))
  (bind _staticmesh (Variables|Default|GetStaticMesh))
  (bind _balloon_hitbox (Variables|Default|GetBalloon_Hitbox))
  (bind (_x _y _z) (Math|Vector|BreakVector _returnvalue))
  (bind _returnvalue_2 (Transformation|GetWorldLocation _balloon_hitbox))
  (Utilities|FlowControl|DoOnce false
    (:Completed
      (Collision|SetCollisionEnabled (Variables|Default|GetBalloon_Hitbox) "NoCollision")
      (if (Variables|Default|GetBalloon_Popped)
        (|CallParentFunction)
        (else
          (Rendering|Material|SetMaterial _staticmesh 0 "/Game/SpyroContent/Global_Assets/Global_Materials/Material_Instances/Invisible_Mat.Invisible_Mat")
          (Rendering|Material|SetMaterial _staticmesh 1 "/Game/SpyroContent/Global_Assets/Global_Materials/Material_Instances/Invisible_Mat.Invisible_Mat")
          (bind _outhit (Collision|LineTraceForObjects _returnvalue (Math|Vector|MakeVector _x _y (- _z 1e+04)) (Utilities|Array|MakeArray "ObjectTypeQuery1") false 0 "None"))
          (if (.bblockinghit _outhit)
            (Variables|Default|SetFloor_Z_Loc (.Z (Math|Vector|BreakVector (.location _outhit))))
            (Variables|Default|SetBalloon_Popped true)
            (Audio|PlaySoundatLocation "/Game/SpyroContent/Global_Assets/Global_Level_Items/Treasure_Containers/Balloon_Vase/Audio/balloon_pop.balloon_pop" _returnvalue_2 "0, 0, 0" 1.0 1.0 0.0 0 0 0)
            (Effects|SpawnEmitteratLocation "/Game/SpyroContent/Global_Assets/Global_Level_Items/Treasure_Containers/Balloon_Vase/Balloon_Burst.Balloon_Burst" _returnvalue_2)
            (else
              (Development|PrintString "Balloon Vase failed to find a floor. Your gem's gonna fall forever!"))))))))

(event EventTick
  (params (DeltaSeconds :type Float%20%28single-precision%29))
  (bind _returnvalue (Transformation|GetActorLocation))
  (bind _floor_z_loc (Variables|Default|GetFloor_Z_Loc))
  (bind _returnvalue_2 (+ _floor_z_loc 2e+01))
  (if (and (Variables|Default|GetBalloon_Popped) (not (Variables|Default|GetContainer_Destroyed)))
    (if (> (.z (Transformation|GetActorLocation)) _returnvalue_2)
      (Transformation|AddActorWorldOffset (Math|Vector|MakeVector 0.0 0.0 (* -8e+02 (Utilities|Time|GetWorldDeltaSeconds))))
      (else
        (Utilities|FlowControl|DoOnce false
          (:Completed
            (Transformation|SetActorLocation (Math|Vector|MakeVector (.x _returnvalue) (.y _returnvalue) _returnvalue_2) false false)
            (Variables|/Game/SpyroContent/Global_Assets/Global_Components/Drops_Items.Drops_Items_C|SetCannot_Drop_Items (Variables|Default|GetItem_Drop_Component) false)
            (CallFunction|ResetonDamaged)
            (Default|DealDamage (Variables|Default|GetDamageable) "NewEnumerator0" "0, 0, 0" false 0 false)))))))

(event EventResetThisContainer
  (bind _returnvalue (Transformation|GetActorLocation))
  (bind _staticmesh (Variables|Default|GetStaticMesh))
  (|CallParentFunction)
  (Variables|Default|SetBalloon_Popped false)
  (CallFunction|ResetonDamaged)
  (CallFunction|ResetonVaseHitsFloor)
  (Collision|SetCollisionEnabled (Variables|Default|GetBalloon_Hitbox) "QueryAndPhysics")
  (Rendering|Material|SetMaterial _staticmesh 0 "/Game/SpyroContent/Global_Assets/Global_Materials/Material_Instances/Untex_Vertex_Color.Untex_Vertex_Color")
  (Rendering|Material|SetMaterial _staticmesh 1 "/Game/SpyroContent/Global_Assets/Global_Level_Items/Treasure_Containers/Balloon_Vase/Materials/Balloon_Vase_Mat.Balloon_Vase_Mat")
  (Transformation|SetActorLocation (Math|Vector|MakeVector (.x _returnvalue) (.y _returnvalue) (Variables|Default|GetStarting_Z_Loc)) false false)
  (CallFunction|BalloonFloatUp)
  (Variables|/Game/SpyroContent/Global_Assets/Global_Components/Drops_Items.Drops_Items_C|SetCannot_Drop_Items (Variables|Default|GetItem_Drop_Component) true))

(fn ConstructionScript
  (|CallParentFunction))