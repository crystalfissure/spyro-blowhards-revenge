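; Butterfly jar treasure container for Spyro levels, showing a spinning butterfly with particles until it is successfully damaged.
; Builds on a parent container class, hiding the butterfly mesh and particles on damage and showing them when the container turns visible.
; When the item drop component finishes, each dropped Blue Butterfly receives a unique name derived from the jar, plus the jar's level item index and skill level award.
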(event Custom|Manage%20Dropped%20Butterfly
  (for _array_element (Variables|/Game/SpyroContent/Global_Assets/Global_Components/Drops_Items.Drops_Items_C|GetItems_I_Dropped (Variables|Default|GetItem_Drop_Component))
    (bind _asblue_butterfly_bp (Utilities|Casting|CastToBlue_Butterfly_BP _array_element))
    (Utilities|IsValid _asblue_butterfly_bp
      (:Is%20Valid
        (Variables|/Game/SpyroContent/Global_Assets/Global_Level_Items/Butterflies/Actors/Blue_Butterfly_BP.Blue_Butterfly_BP_C|SetMy_Unique_Name _asblue_butterfly_bp (Utilities|String|Append (Utilities|GetObjectName self) " " "0"))
        (Variables|/Game/SpyroContent/Global_Assets/Global_Level_Items/Butterflies/Actors/Blue_Butterfly_BP.Blue_Butterfly_BP_C|SetLevel%20Item%20Index _asblue_butterfly_bp (Variables|Default|GetLevel%20Item%20Index))
        (Variables|/Game/SpyroContent/Global_Assets/Global_Level_Items/Butterflies/Actors/Blue_Butterfly_BP.Blue_Butterfly_BP_C|SetSkill%20Level%20Award _asblue_butterfly_bp (Variables|Default|GetSkill%20Level%20Award))))))

(event Custom|Container%20is%20Visible
  (Rendering|SetVisibility (Variables|Default|GetButterfly_Mesh) true false))

(event EventBeginPlay
  (|CallParentFunction)
  (EventDispatchers|BindEventtoFinishedDroppingItems (Variables|Default|GetItem_Drop_Component) (delegate Custom|Manage%20Dropped%20Butterfly))
  (EventDispatchers|BindEventtoContainerTurnedVisible self (delegate Custom|Container%20is%20Visible)))

(event EventTreasureContainerSuccessfullyDamaged
  (|CallParentFunction)
  (Rendering|SetVisibility (Variables|Default|GetButterfly_Mesh) false false))

(event EventTick
  (params (DeltaSeconds :type Float%20%28single-precision%29))
  (|CallParentFunction DeltaSeconds)
  (Transformation|AddRelativeRotation (Variables|Default|GetButterfly_Mesh) (Math|Rotator|MakeRotator 0.0 0.0 (* DeltaSeconds -8e+01)) false false))

(fn ConstructionScript
  (|CallParentFunction))