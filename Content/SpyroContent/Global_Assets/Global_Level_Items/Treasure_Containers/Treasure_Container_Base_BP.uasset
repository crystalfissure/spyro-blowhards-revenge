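; Base Blueprint for breakable treasure containers, which burst into shards when damaged and drop items.
; Damageable component events drive the wobble, metal heat tint via dynamic materials, and breaking, which hides the container and spawns a burst actor with sound.
; An ItemDropComponent reset restores visibility and collision if items remain to drop.
; A save-data option swaps between S1 and S23 skins, also selecting shard meshes and break sound.
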(event Custom|Deal%20Damage%20to%20Treasure%20Container
  (if (and (not (Variables|Default|GetContainer_Destroyed)) (not (Variables|/Game/SpyroContent/Global_Assets/Global_Components/Damageable_Com.Damageable_Com_C|GetInvincible (Variables|Default|GetDamageable))))
    (Default|CallDamageWasSuccessfullyDealt (Variables|Default|GetDamageable))))

(event Custom|Wobble
  (if (Variables|Default|GetWobbles)
    (Utilities|FlowControl|DoOnce false :!label _label
      (:Completed
        (bind _newtrack_0 (Timeline|Timeline_0 PlayFromStart)
          (:Update
            (Transformation|SetRelativeRotation (Variables|Default|GetStaticMesh) (Math|Rotator|MakeRotator 0.0 _newtrack_0 0.0) false false))
          (:Finished
            (goto _label Reset)))))))

(event EventBeginPlay
  (bind _damageable (Variables|Default|GetDamageable))
  (bind _staticmesh (Variables|Default|GetStaticMesh))
  (Variables|/Game/SpyroContent/Global_Assets/Global_Components/Damageable_Com.Damageable_Com_C|SetObject's%20Hitbox%20Component (Variables|Default|GetDamageable) (Variables|Default|GetCapsule%20Component))
  (Variables|Default|SetS2&3_Mesh (Variables|/Script/Engine.StaticMeshComponent|GetStaticMesh _staticmesh))
  (Variables|Default|SetS2&3%20Materials (Rendering|Material|GetMaterials _staticmesh))
  (Variables|Default|SetCharging%20Attacker%20Default%20Response (Collision|GetCollisionResponsetoChannel (Variables|Default|GetCapsule%20Component) "ECC_GameTraceChannel4"))
  (EventDispatchers|BindEventtoCallDealDamage _damageable (delegate Custom|Deal%20Damage%20to%20Treasure%20Container))
  (EventDispatchers|BindEventtoDamageWasAttempted _damageable (delegate Custom|Wobble))
  (EventDispatchers|BindEventtoHeatMetal (Variables|Default|GetDamageable) (delegate HeattheMetal))
  (EventDispatchers|BindEventtoDamageWasSuccessfullyDealt (Variables|Default|GetDamageable) (delegate OnDamageSuccessfullyDealt))
  (EventDispatchers|BindEventtoItemDropperSuccessfullyReset (Variables|Default|GetItem_Drop_Component) (|ResetTreasureContainer))
  (if (not (Variables|Spyro1|GetNo%20S1%20Form))
    (bind _asspyro_persistant_data (Utilities|Casting|CastToSpyro_PersistantData (Game|GetGameInstance)))
    (EventDispatchers|BindEventtoChangeTreasureSkins _asspyro_persistant_data (delegate TreasureSkin))
    (Utilities|FlowControl|Delay 0.2)
    (CallFunction|SetSkin)))

(fn ConstructionScript
  (|CallParentFunction))

(event Custom|Reset%20Heat%20Metal
  (bind _damageable (Variables|Default|GetDamageable))
  (bind _component_with_metal_material (Variables|/Game/SpyroContent/Global_Assets/Global_Components/Damageable_Com.Damageable_Com_C|GetComponent_with_Metal_Material _damageable))
  (Utilities|FlowControl|DoOnce false) ; enters at Reset
)

(event Custom|Heat%20Metal
  (bind _damageable (Variables|Default|GetDamageable))
  (bind _component_with_metal_material (Variables|/Game/SpyroContent/Global_Assets/Global_Components/Damageable_Com.Damageable_Com_C|GetComponent_with_Metal_Material _damageable))
  (bind _component_with_metal_material_2 (Variables|/Game/SpyroContent/Global_Assets/Global_Components/Damageable_Com.Damageable_Com_C|GetComponent_with_Metal_Material (Variables|Default|GetDamageable))
    (:then
      (Utilities|FlowControl|DoOnce false
        (:Completed
          (Utilities|Array|Clear (Variables|Default|GetDyn_Mat_Refs))
          (if (and (Variables|Spyro1|GetS1_Mode) (not (Variables|Spyro1|GetNo%20S1%20Form)))
            (for (_array_element _array_index) (Variables|Spyro1|GetS1_Mats)
              (if (>= (Utilities|Array|FindItem (Variables|/Game/SpyroContent/Global_Assets/Global_Components/Damageable_Com.Damageable_Com_C|GetMetal%20Material%20Indexes (Variables|Default|GetDamageable)) _array_index) 0)
                (bind _returnvalue (Rendering|Material|CreateDynamicMaterialInstance (Variables|/Game/SpyroContent/Global_Assets/Global_Components/Damageable_Com.Damageable_Com_C|GetComponent_with_Metal_Material (Variables|Default|GetDamageable)) _array_index _array_element "None" :!class /Script/Engine.PrimitiveComponent))
                (Utilities|Array|Add (Variables|Default|GetDyn_Mat_Refs) _returnvalue)))
            (Utilities|FlowControl|Sequence
              (:then_0
                (bind _newtrack_0 (Timeline|Timeline_2 PlayFromStart)
                  (:Update
                    (for _array_element_2 (Variables|Default|GetDyn_Mat_Refs)
                      (Rendering|Material|SetVectorParameterValue _array_element_2 "ColorChange" (Utilities|Struct|MakeLinearColor (.x _newtrack_0) (.y _newtrack_0) (.z _newtrack_0) 0.0) :!class /Script/Engine.MaterialInstanceDynamic)))))
              (:then_1
                (Utilities|FlowControl|Delay 1.0)
                (CallFunction|ResetHeatMetal)))
            (else
              (for (_ _array_index_2) (Rendering|Material|GetMaterials _component_with_metal_material_2)
                (if (>= (Utilities|Array|FindItem (Variables|/Game/SpyroContent/Global_Assets/Global_Components/Damageable_Com.Damageable_Com_C|GetMetal%20Material%20Indexes (Variables|Default|GetDamageable)) _array_index_2) 0)
                  (bind _returnvalue_2 (Rendering|Material|CreateDynamicMaterialInstance _component_with_metal_material _array_index_2 (Rendering|Material|GetMaterial _component_with_metal_material _array_index_2) "None" :!class /Script/Engine.PrimitiveComponent))
                  (Utilities|Array|Add (Variables|Default|GetDyn_Mat_Refs) _returnvalue_2)))
              (Utilities|FlowControl|Sequence
                (:then_0
                  (bind _newtrack_0_2 (Timeline|Timeline_1 PlayFromStart)
                    (:Update
                      (for _array_element_3 (Variables|Default|GetDyn_Mat_Refs)
                        (Rendering|Material|SetVectorParameterValue _array_element_3 "ColorChange" (Utilities|Struct|MakeLinearColor (.x _newtrack_0_2) (.y _newtrack_0_2) (.z _newtrack_0_2) 0.0) :!class /Script/Engine.MaterialInstanceDynamic)))))
                (:then_1
                  (Utilities|FlowControl|Delay 1.0)
                  (CallFunction|ResetHeatMetal))))))))
    (:else)))

(event Custom|Set%20Skin
  (bind _staticmesh (Variables|Default|GetStaticMesh))
  (bind _asspyro_save_data (CallFunction|LoadSpyroGame self))
  (Utilities|IsValid _asspyro_save_data
    (:Is%20Valid
      (Variables|Spyro1|SetS1_Mode (Variables|/Game/SpyroContent/Global_Assets/Global_SaveData/Spyro_SaveData.Spyro_SaveData_C|GetS1_Treasure _asspyro_save_data))
      (if (not (== _staticmesh (select (Variables|/Game/SpyroContent/Global_Assets/Global_SaveData/Spyro_SaveData.Spyro_SaveData_C|GetS1_Treasure _asspyro_save_data) (Variables|Spyro1|GetS1_StaticMesh) (Variables|Default|GetS2&3_Mesh))))
        (Components|StaticMesh|SetStaticMesh _staticmesh (select (Variables|/Game/SpyroContent/Global_Assets/Global_SaveData/Spyro_SaveData.Spyro_SaveData_C|GetS1_Treasure _asspyro_save_data) (Variables|Spyro1|GetS1_StaticMesh) (Variables|Default|GetS2&3_Mesh)))
        (if (Variables|/Game/SpyroContent/Global_Assets/Global_SaveData/Spyro_SaveData.Spyro_SaveData_C|GetS1_Treasure _asspyro_save_data)
          (for (_array_element _array_index) (Variables|Spyro1|GetS1_Mats)
            (Rendering|Material|SetMaterial (Variables|Default|GetStaticMesh) _array_index _array_element))
          (else
            (for (_array_element_2 _array_index_2) (Variables|Default|GetS2&3%20Materials)
              (Rendering|Material|SetMaterial (Variables|Default|GetStaticMesh) _array_index_2 _array_element_2))))))))

(event Custom|Treasure%20Container%20Successfully%20Damaged
  (bind _damageable (Variables|Default|GetDamageable))
  (bind _capsule_component (Variables|Default|GetCapsule%20Component))
  (bind _s1_mode (Variables|Spyro1|GetS1_Mode))
  (bind _deal_damage___damage_type (Variables|/Game/SpyroContent/Global_Assets/Global_Components/Damageable_Com.Damageable_Com_C|GetDeal%20Damage%20-%20Damage%20Type _damageable))
  (Rendering|SetVisibility (Variables|Default|GetStaticMesh) false false)
  (Collision|SetCollisionResponsetoAllChannels _capsule_component "ECR_Ignore")
  (Collision|SetCollisionObjectType _capsule_component "ECC_PhysicsBody")
  (Variables|Default|SetContainer_Destroyed true)
  (Default|CallContainerSuccessfullyDamaged)
  (bind _returnvalue (Game|SpawnActorfromClass "/Game/SpyroContent/Global_Assets/Global_Level_Items/Treasure_Containers/Basket/Actors/Basket_Burst_BP.Basket_Burst_BP_C" (Transformation|GetActorTransform) "AlwaysSpawn" 0 0))
  (Default|ShardBurstAction _returnvalue (select _s1_mode (Variables|Spyro1|GetS1_Shard%20Mesh%201) (Variables|Default|GetShard%20Mesh%201)) (select _s1_mode (Variables|Spyro1|GetS1_Shard%20Mesh%202) (Variables|Default|GetShard%20Mesh%202)))
  (Audio|PlaySoundatLocation (select (Variables|Spyro1|GetS1_Mode) (Variables|Spyro1|GetS1_Break_Sound) (Variables|Default|GetBreak_Sound)) (Transformation|GetActorLocation) "0, 0, 0" 1.0 1.0 0.0 0 0 0)
  (if (or (Utilities|Enum|Equal(Enum) _deal_damage___damage_type "NewEnumerator1") (Utilities|Enum|Equal(Enum) _deal_damage___damage_type "NewEnumerator3"))
    (Default|ActivateBlackSmoke _returnvalue)))

(event Custom|Reset%20This%20Container
  (bind _capsule_component (Variables|Default|GetCapsule%20Component))
  (bind _i_can_drop_items (Default|ShouldIDropAnyItems? (Variables|Default|GetItem_Drop_Component)))
  (if _i_can_drop_items
    (Default|CallContainerTurnedVisible)
    (Rendering|SetVisibility (Variables|Default|GetStaticMesh) true false)
    (Collision|SetCollisionResponsetoAllChannels _capsule_component "ECR_Block")
    (Collision|SetCollisionObjectType _capsule_component "ECC_WorldStatic")
    (Collision|SetCollisionResponsetoChannel _capsule_component "ECC_GameTraceChannel1" "ECR_Ignore")
    (Collision|SetCollisionResponsetoChannel _capsule_component "ECC_GameTraceChannel3" "ECR_Ignore")
    (Collision|SetCollisionResponsetoChannel _capsule_component "ECC_GameTraceChannel1" "ECR_Ignore")
    (Collision|SetCollisionResponsetoChannel _capsule_component "ECC_GameTraceChannel4" (Variables|Default|GetCharging%20Attacker%20Default%20Response))
    (Collision|SetCollisionResponsetoChannel _capsule_component "ECC_GameTraceChannel5" "ECR_Ignore")
    (Variables|Default|SetContainer_Destroyed false)))