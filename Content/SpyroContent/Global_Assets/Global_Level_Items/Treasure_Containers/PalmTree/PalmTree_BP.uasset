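; Palm tree Blueprint, filed under treasure containers, that plays a wood-hit sound when something tries to damage it.
; On BeginPlay it binds one handler to its Damageable component's events for both resisted and successfully dealt damage.
; The handler plays the sound at the actor's location, using a DoOnce that resets after a short delay to throttle repeated hits.
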(event Custom|When%20Damage%20is%20Attempted
  (Utilities|FlowControl|DoOnce false :!label _label
    (:Completed
      (Audio|PlaySoundatLocation "/Game/SpyroContent/Global_Assets/Global_Level_Items/Treasure_Containers/PalmTree/WOOD_HIT.WOOD_HIT" (Transformation|GetActorLocation) "0, 0, 0" 1.0 1.0 0.0 0 0 0)
      (Utilities|FlowControl|Delay 1.0)
      (goto _label Reset))))

(event EventBeginPlay
  (bind _damageable (Variables|Default|GetDamageable))
  (|CallParentFunction)
  (EventDispatchers|BindEventtoDamageWasAttemptedButI'mResistant _damageable (delegate Custom|When%20Damage%20is%20Attempted))
  (EventDispatchers|BindEventtoDamageWasSuccessfullyDealt _damageable (delegate Custom|When%20Damage%20is%20Attempted)))

(fn ConstructionScript
  (|CallParentFunction))