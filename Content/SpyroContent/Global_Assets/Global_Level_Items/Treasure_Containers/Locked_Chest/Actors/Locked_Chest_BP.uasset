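; Locked treasure chest that opens with a collected key, or hides a loose or carried key if broken without one.
; Overlap saves key and chest names per save slot, then plays a skippable unlock cutscene with input locked and a spawned key unlocker.
; Unlocking clears Invincible and deals super damage, so ticking Invincible makes it key-only.
; On BeginPlay or reset it re-unlocks saved chests, waiting for any portal transition.
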(event OnComponentBeginOverlap(Box)
  (params (OverlappedComponent :type Primitive%20Component%20Object%20Reference) (OtherActor :type Actor%20Object%20Reference) (OtherComp :type Primitive%20Component%20Object%20Reference) (OtherBodyIndex :type Integer) (bFromSweep :type Boolean) (SweepResult :type Hit%20Result%20Structure%20%28by%20ref%29))
  (bind _asbp_base_playable (Utilities|Casting|CastToBP_Base_Playable OtherActor))
  (if (Math|Boolean|ANDBoolean (== (Variables|/Script/Engine.Character|GetCapsuleComponent _asbp_base_playable) OtherComp) (not (Variables|Default|GetContainer_Destroyed)) (not (Variables|/Game/SpyroContent/Global_Assets/Global_Characters/Playable_Characters/BP_Base_Playable.BP_Base_Playable_C|GetDid%20we%20disable%20input? _asbp_base_playable)) (not (Variables|Default|GetContainer%20Unlocked)))
    (bind _array_element (Utilities|Array|ForEachLoopwithBreak (Variables|/Game/SpyroContent/Global_Assets/Global_Characters/Playable_Characters/BP_Base_Playable.BP_Base_Playable_C|GetMy%20Collected%20Keys _asbp_base_playable) :!label _label)
      (:LoopBody
        (Utilities|IsValid _array_element
          (:Is%20Valid
            (Utilities|FlowControl|Sequence
              (:then_0
                (|SaveKeyandChestNames _array_element
                  (:then_1
                    (bind _output_get (Variables|Default|SetPlayer%20Opening%20Me _asbp_base_playable))
                    (Input|DisableInput _asbp_base_playable (Variables|/Game/SpyroContent/Global_Assets/Global_Characters/Playable_Characters/BP_Base_Playable.BP_Base_Playable_C|GetSpyroContr_Ref _asbp_base_playable))
                    (Input|EnableInput (Variables|/Game/SpyroContent/Global_Assets/Global_Characters/Playable_Characters/BP_Base_Playable.BP_Base_Playable_C|GetSpyroContr_Ref _asbp_base_playable))
                    (EventDispatchers|BindEventtoPlayerDied _output_get (delegate Custom|Died%20While%20Unlocking%20Chest))
                    (Variables|/Game/SpyroContent/Global_Assets/Global_Characters/Playable_Characters/BP_Base_Playable.BP_Base_Playable_C|SetDid%20we%20disable%20input? _asbp_base_playable true)
                    (Default|ShowBlackBars (Variables|/Game/SpyroContent/Global_Assets/Global_Characters/Playable_Characters/BP_Base_Playable.BP_Base_Playable_C|GetSpyroContr_Ref _asbp_base_playable))
                    (Actor|DestroyActor _array_element)
                    (Utilities|Array|RemoveItem (Variables|/Game/SpyroContent/Global_Assets/Global_Characters/Playable_Characters/BP_Base_Playable.BP_Base_Playable_C|GetMy%20Collected%20Keys _asbp_base_playable) _array_element)
                    (Default|SetHUDNumberOfKeys (Variables|/Game/SpyroContent/Global_Assets/Global_Characters/Playable_Characters/Spyro_PlayerController.Spyro_PlayerController_C|GetMy_HUD_Ref (Variables|/Game/SpyroContent/Global_Assets/Global_Characters/Playable_Characters/BP_Base_Playable.BP_Base_Playable_C|GetSpyroContr_Ref _asbp_base_playable)) (- (Variables|/Game/SpyroContent/Global_Assets/Global_UserInterface/Widgets/HUD.HUD_C|GetHUD_NumberOfKeys (Variables|/Game/SpyroContent/Global_Assets/Global_Characters/Playable_Characters/Spyro_PlayerController.Spyro_PlayerController_C|GetMy_HUD_Ref (Variables|/Game/SpyroContent/Global_Assets/Global_Characters/Playable_Characters/BP_Base_Playable.BP_Base_Playable_C|GetSpyroContr_Ref _asbp_base_playable))) 1))
                    (Variables|/Game/SpyroContent/Global_Assets/Global_Characters/Playable_Characters/BP_Base_Playable.BP_Base_Playable_C|SetPlayer_State (Variables|Default|GetPlayer%20Opening%20Me) "NewEnumerator0")
                    (Components|Movement|StopMovementImmediately (Variables|/Script/Engine.Character|GetCharacterMovement (Variables|Default|GetPlayer%20Opening%20Me)))
                    (bind _returnvalue (Game|SpawnActorfromClass "/Game/SpyroContent/Global_Assets/Global_Level_Items/Treasure_Containers/Locked_Chest/Actors/Key_Unlocking_BP.Key_Unlocking_BP_C" (Transformation|GetActorTransform) "AlwaysSpawn" 0 0))
                    (bind _output_get_2 (Variables|Default|SetMy%20Key%20Unlocker _returnvalue))
                    (bind _player_opening_me (Variables|Default|GetPlayer%20Opening%20Me)
                      (:then
                        (Variables|/Game/SpyroContent/Global_Assets/Global_Characters/Playable_Characters/BP_Base_Playable.BP_Base_Playable_C|SetLookAt_Target_SocketName _player_opening_me "Key")
                        (Variables|/Game/SpyroContent/Global_Assets/Global_Characters/Playable_Characters/BP_Base_Playable.BP_Base_Playable_C|SetLookAt_Target _player_opening_me (Variables|/Game/SpyroContent/Global_Assets/Global_Level_Items/Treasure_Containers/Locked_Chest/Actors/Key_Unlocking_BP.Key_Unlocking_BP_C|GetSkeletalMesh _output_get_2)))
                      (:else
                        _))
                    (Utilities|FlowControl|Delay 2.0)
                    (if (and (not (Variables|Default|GetSkipped%20My%20Cutscene)) (not (Variables|Default|GetContainer_Destroyed)))
                      (CallFunction|UnlockChest)))))
              (:then_1
                (goto _label Break)))))))))

(event Custom|try%20again
  (Utilities|FlowControl|Delay 1.0)
  (bind _asspyro_persistant_data (Utilities|Casting|CastToSpyro_PersistantData (Game|GetGameInstance)))
  (bind _returnvalue (SaveGame|LoadGamefromSlot (Variables|/Game/SpyroContent/Global_Assets/Global_SaveData/Spyro_PersistantData.Spyro_PersistantData_C|GetCurrent_Level_Name _asspyro_persistant_data)))
  (bind _asindividual_level_save_data (Utilities|Casting|CastToIndividual_Level_SaveData _returnvalue))
  (for _array_element (Utilities|Select :Index (Variables|/Game/SpyroContent/Global_Assets/Global_SaveData/Spyro_PersistantData.Spyro_PersistantData_C|GetCurrent_SaveSlot _asspyro_persistant_data) :Option%200 (Variables|/Game/SpyroContent/Global_Assets/Global_SaveData/Individual_Level_SaveData.Individual_Level_SaveData_C|GetLockedChests_Opened_0 _asindividual_level_save_data) :Option%201 (Variables|/Game/SpyroContent/Global_Assets/Global_SaveData/Individual_Level_SaveData.Individual_Level_SaveData_C|GetLockedChests_Opened_1 _asindividual_level_save_data) :Option%202 (Variables|/Game/SpyroContent/Global_Assets/Global_SaveData/Individual_Level_SaveData.Individual_Level_SaveData_C|GetLockedChests_Opened_2 _asindividual_level_save_data) :Option%203 (Variables|/Game/SpyroContent/Global_Assets/Global_SaveData/Individual_Level_SaveData.Individual_Level_SaveData_C|GetLockedChests_Opened_3 _asindividual_level_save_data) :Option%204 (Variables|/Game/SpyroContent/Global_Assets/Global_SaveData/Individual_Level_SaveData.Individual_Level_SaveData_C|GetLockedChests_Opened_4 _asindividual_level_save_data) :Option%205 (Variables|/Game/SpyroContent/Global_Assets/Global_SaveData/Individual_Level_SaveData.Individual_Level_SaveData_C|GetLockedChests_Opened_5 _asindividual_level_save_data))
    (if (Utilities|Enum|Equal(Enum) _array_element (Utilities|GetObjectName self))
      (if (Variables|/Game/SpyroContent/Global_Assets/Global_SaveData/Spyro_PersistantData.Spyro_PersistantData_C|GetPortal_Transition _asspyro_persistant_data)
        (EventDispatchers|BindEventtoPortalTransitionEnded _asspyro_persistant_data (delegate Custom|portal%20transition%20ended,%20unlock%20chest))
        (else
          (CallFunction|UnlockChest))))))

(event Custom|Died%20While%20Unlocking%20Chest
  (bind _player_opening_me (Variables|Default|GetPlayer%20Opening%20Me)
    (:then
      (Input|DisableInput (Variables|/Game/SpyroContent/Global_Assets/Global_Characters/Playable_Characters/BP_Base_Playable.BP_Base_Playable_C|GetSpyroContr_Ref _player_opening_me))
      (Default|HideBlackBars (Variables|/Game/SpyroContent/Global_Assets/Global_Characters/Playable_Characters/BP_Base_Playable.BP_Base_Playable_C|GetSpyroContr_Ref _player_opening_me)))
    (:else
      _))
  (CallFunction|ClearPlayerOpeningMe))

(event Custom|Clear%20Player%20Opening%20Me
  (bind _player_opening_me (Variables|Default|GetPlayer%20Opening%20Me)
    (:then
      (EventDispatchers|UnbindEventfromPlayerDied _player_opening_me (delegate Custom|Died%20While%20Unlocking%20Chest))
      (Variables|/Game/SpyroContent/Global_Assets/Global_Characters/Playable_Characters/BP_Base_Playable.BP_Base_Playable_C|SetLookAt_Target_SocketName _player_opening_me "None")
      (Variables|/Game/SpyroContent/Global_Assets/Global_Characters/Playable_Characters/BP_Base_Playable.BP_Base_Playable_C|SetLookAt_Target _player_opening_me 0))
    (:else
      _))
  (Variables|Default|SetPlayer%20Opening%20Me 0))

(event Custom|portal%20transition%20ended,%20unlock%20chest
  (Utilities|FlowControl|Delay 2.0)
  (CallFunction|UnlockChest))

(event EventBeginPlay
  (|CallParentFunction)
  (Utilities|FlowControl|Delay 1.0)
  (bind _asspyro_persistant_data (Utilities|Casting|CastToSpyro_PersistantData (Game|GetGameInstance)))
  (bind _returnvalue (SaveGame|LoadGamefromSlot (Variables|/Game/SpyroContent/Global_Assets/Global_SaveData/Spyro_PersistantData.Spyro_PersistantData_C|GetCurrent_Level_Name _asspyro_persistant_data)))
  (bind _asindividual_level_save_data (Utilities|Casting|CastToIndividual_Level_SaveData _returnvalue))
  (for _array_element (Utilities|Select :Index (Variables|/Game/SpyroContent/Global_Assets/Global_SaveData/Spyro_PersistantData.Spyro_PersistantData_C|GetCurrent_SaveSlot _asspyro_persistant_data) :Option%200 (Variables|/Game/SpyroContent/Global_Assets/Global_SaveData/Individual_Level_SaveData.Individual_Level_SaveData_C|GetLockedChests_Opened_0 _asindividual_level_save_data) :Option%201 (Variables|/Game/SpyroContent/Global_Assets/Global_SaveData/Individual_Level_SaveData.Individual_Level_SaveData_C|GetLockedChests_Opened_1 _asindividual_level_save_data) :Option%202 (Variables|/Game/SpyroContent/Global_Assets/Global_SaveData/Individual_Level_SaveData.Individual_Level_SaveData_C|GetLockedChests_Opened_2 _asindividual_level_save_data) :Option%203 (Variables|/Game/SpyroContent/Global_Assets/Global_SaveData/Individual_Level_SaveData.Individual_Level_SaveData_C|GetLockedChests_Opened_3 _asindividual_level_save_data) :Option%204 (Variables|/Game/SpyroContent/Global_Assets/Global_SaveData/Individual_Level_SaveData.Individual_Level_SaveData_C|GetLockedChests_Opened_4 _asindividual_level_save_data) :Option%205 (Variables|/Game/SpyroContent/Global_Assets/Global_SaveData/Individual_Level_SaveData.Individual_Level_SaveData_C|GetLockedChests_Opened_5 _asindividual_level_save_data))
    (if (Utilities|Enum|Equal(Enum) _array_element (Utilities|GetObjectName self))
      (if (Variables|/Game/SpyroContent/Global_Assets/Global_SaveData/Spyro_PersistantData.Spyro_PersistantData_C|GetPortal_Transition _asspyro_persistant_data)
        (EventDispatchers|BindEventtoPortalTransitionEnded _asspyro_persistant_data (delegate Custom|portal%20transition%20ended,%20unlock%20chest))
        (else
          (CallFunction|UnlockChest))))))

(event EventTick
  (params (DeltaSeconds :type Float%20%28single-precision%29))
  (bind _player_opening_me (Variables|Default|GetPlayer%20Opening%20Me)
    (:then
      (if (and (Variables|/Game/SpyroContent/Global_Assets/Global_Characters/Playable_Characters/BP_Base_Playable.BP_Base_Playable_C|GetDid%20we%20disable%20input? _player_opening_me) (Utilities|Enum|Equal(Enum) (Variables|/Game/SpyroContent/Global_Assets/Global_Characters/Playable_Characters/BP_Base_Playable.BP_Base_Playable_C|GetEnvironmental_State _player_opening_me) "NewEnumerator0"))
        (Transformation|SetActorRotation (Variables|Default|GetPlayer%20Opening%20Me) (Math|Rotator|Lerp(Rotator) (Transformation|GetActorRotation (Variables|Default|GetPlayer%20Opening%20Me)) (Math|Rotator|FindLookatRotation (Transformation|GetActorLocation (Variables|Default|GetPlayer%20Opening%20Me)) (Transformation|GetActorLocation)) (* (Utilities|Time|GetWorldDeltaSeconds) 1e+01) true))))
    (:else)))

(event EventResetThisContainer
  (|CallParentFunction)
  (bind _key_i_have_hidden (Variables|Default|GetKey%20I%20Have%20Hidden)
    (:then
      (Default|ResetKey _key_i_have_hidden)
      (Variables|Default|SetKey%20I%20Have%20Hidden 0))
    (:else
      _))
  (Utilities|FlowControl|Delay 1.0)
  (bind _asspyro_persistant_data (Utilities|Casting|CastToSpyro_PersistantData (Game|GetGameInstance)))
  (bind _returnvalue (SaveGame|LoadGamefromSlot (Variables|/Game/SpyroContent/Global_Assets/Global_SaveData/Spyro_PersistantData.Spyro_PersistantData_C|GetCurrent_Level_Name _asspyro_persistant_data)))
  (bind _asindividual_level_save_data (Utilities|Casting|CastToIndividual_Level_SaveData _returnvalue))
  (for _array_element (Utilities|Select :Index (Variables|/Game/SpyroContent/Global_Assets/Global_SaveData/Spyro_PersistantData.Spyro_PersistantData_C|GetCurrent_SaveSlot _asspyro_persistant_data) :Option%200 (Variables|/Game/SpyroContent/Global_Assets/Global_SaveData/Individual_Level_SaveData.Individual_Level_SaveData_C|GetLockedChests_Opened_0 _asindividual_level_save_data) :Option%201 (Variables|/Game/SpyroContent/Global_Assets/Global_SaveData/Individual_Level_SaveData.Individual_Level_SaveData_C|GetLockedChests_Opened_1 _asindividual_level_save_data) :Option%202 (Variables|/Game/SpyroContent/Global_Assets/Global_SaveData/Individual_Level_SaveData.Individual_Level_SaveData_C|GetLockedChests_Opened_2 _asindividual_level_save_data) :Option%203 (Variables|/Game/SpyroContent/Global_Assets/Global_SaveData/Individual_Level_SaveData.Individual_Level_SaveData_C|GetLockedChests_Opened_3 _asindividual_level_save_data) :Option%204 (Variables|/Game/SpyroContent/Global_Assets/Global_SaveData/Individual_Level_SaveData.Individual_Level_SaveData_C|GetLockedChests_Opened_4 _asindividual_level_save_data) :Option%205 (Variables|/Game/SpyroContent/Global_Assets/Global_SaveData/Individual_Level_SaveData.Individual_Level_SaveData_C|GetLockedChests_Opened_5 _asindividual_level_save_data))
    (if (Utilities|Enum|Equal(Enum) _array_element (Utilities|GetObjectName self))
      (if (Variables|/Game/SpyroContent/Global_Assets/Global_SaveData/Spyro_PersistantData.Spyro_PersistantData_C|GetPortal_Transition _asspyro_persistant_data)
        (EventDispatchers|BindEventtoPortalTransitionEnded _asspyro_persistant_data (delegate Custom|portal%20transition%20ended,%20unlock%20chest))
        (else
          (CallFunction|UnlockChest))))))

(event EventTreasureContainerSuccessfullyDamaged
  (|CallParentFunction)
  (Utilities|FlowControl|Sequence
    (:then_0
      (if (not (Variables|Default|GetContainer%20Unlocked))
        (Development|PrintString "you broke me without using a key, so now one of this levels keys MUST be hidden! You cannot collect spare keys!!!" true true "(R=0.000000,G=0.660000,B=1.000000,A=1.000000)" 3e+01)
        (bind _outactors (Actor|GetAllActorsOfClass "/Game/SpyroContent/Global_Assets/Global_Level_Items/Treasure_Containers/Locked_Chest/Actors/Key_BP.Key_BP_C"))
        (bind _array_element (Utilities|Array|ForEachLoopwithBreak _outactors :!label _label)
          (:LoopBody
            (if (not (Variables|/Game/SpyroContent/Global_Assets/Global_Level_Items/Treasure_Containers/Locked_Chest/Actors/Key_BP.Key_BP_C|GetCollected _array_element))
              (Variables|Default|SetKey%20I%20Have%20Hidden _array_element)
              (Rendering|SetActorHiddenInGame _array_element true)
              (Variables|/Game/SpyroContent/Global_Assets/Global_Level_Items/Treasure_Containers/Locked_Chest/Actors/Key_BP.Key_BP_C|SetCollected _array_element true)
              (goto _label Break)))
          (:Completed
            (Variables|Default|GetKey%20I%20Have%20Hidden
              (:then)
              (:else
                (Development|PrintString "there wasnt a loose key so i took one from your inventory instead" true true "(R=0.000000,G=0.660000,B=1.000000,A=1.000000)" 3e+01)
                (bind _outactors_2 (Actor|GetAllActorsOfClass "/Game/SpyroContent/Global_Assets/Global_Characters/Playable_Characters/BP_Base_Playable.BP_Base_Playable_C"))
                (bind _array_element_2 (Utilities|Array|ForEachLoopwithBreak _outactors_2 :!label _label_2)
                  (:LoopBody
                    (bind _array_element_3 (Utilities|Array|ForEachLoopwithBreak (Variables|/Game/SpyroContent/Global_Assets/Global_Characters/Playable_Characters/BP_Base_Playable.BP_Base_Playable_C|GetMy%20Collected%20Keys _array_element_2) :!label _label_3)
                      (:LoopBody
                        (Utilities|IsValid _array_element_3
                          (:Is%20Valid
                            (Variables|Default|SetKey%20I%20Have%20Hidden _array_element_3)
                            (Default|SetHUDNumberOfKeys (Variables|/Game/SpyroContent/Global_Assets/Global_Characters/Playable_Characters/Spyro_PlayerController.Spyro_PlayerController_C|GetMy_HUD_Ref (Variables|/Game/SpyroContent/Global_Assets/Global_Characters/Playable_Characters/BP_Base_Playable.BP_Base_Playable_C|GetSpyroContr_Ref _array_element_2)) (- (Variables|/Game/SpyroContent/Global_Assets/Global_UserInterface/Widgets/HUD.HUD_C|GetHUD_NumberOfKeys (Variables|/Game/SpyroContent/Global_Assets/Global_Characters/Playable_Characters/Spyro_PlayerController.Spyro_PlayerController_C|GetMy_HUD_Ref (Variables|/Game/SpyroContent/Global_Assets/Global_Characters/Playable_Characters/BP_Base_Playable.BP_Base_Playable_C|GetSpyroContr_Ref _array_element_2))) 1))
                            (Utilities|Array|RemoveItem (Variables|/Game/SpyroContent/Global_Assets/Global_Characters/Playable_Characters/BP_Base_Playable.BP_Base_Playable_C|GetMy%20Collected%20Keys _array_element_2) _array_element_3)
                            (Utilities|FlowControl|Sequence
                              (:then_0
                                (goto _label_3 Break))
                              (:then_1
                                (goto _label_2 Break)))))))))))))))
    (:then_1
      (bind _player_opening_me (Variables|Default|GetPlayer%20Opening%20Me)
        (:then
          (Default|HideBlackBars (Variables|/Game/SpyroContent/Global_Assets/Global_Characters/Playable_Characters/BP_Base_Playable.BP_Base_Playable_C|GetSpyroContr_Ref _player_opening_me))
          (Input|EnableInput _player_opening_me (Variables|/Game/SpyroContent/Global_Assets/Global_Characters/Playable_Characters/BP_Base_Playable.BP_Base_Playable_C|GetSpyroContr_Ref _player_opening_me))
          (Variables|/Game/SpyroContent/Global_Assets/Global_Characters/Playable_Characters/BP_Base_Playable.BP_Base_Playable_C|SetDid%20we%20disable%20input? _player_opening_me false)
          (Input|DisableInput (Variables|/Game/SpyroContent/Global_Assets/Global_Characters/Playable_Characters/BP_Base_Playable.BP_Base_Playable_C|GetSpyroContr_Ref _player_opening_me)))
        (:else
          _))
      (CallFunction|ClearPlayerOpeningMe))))

(event Input|ActionEvents|InputActionPause
  (params (Key :type Key%20Structure :default "None"))
  (:Pressed
    (Development|PrintString "locked chest input")
    (if (not (Variables|Default|GetSkipped%20My%20Cutscene))
      (Variables|Default|SetSkipped%20My%20Cutscene true)
      (CallFunction|UnlockChest)
      (bind _my_key_unlocker (Variables|Default|GetMy%20Key%20Unlocker)
        (:then
          (Actor|DestroyActor _my_key_unlocker))
        (:else)))))

(event Input|ActionEvents|InputActionAim/Talk
  (params (Key :type Key%20Structure :default "None"))
  (:Pressed
    (Development|PrintString "locked chest input")
    (if (not (Variables|Default|GetSkipped%20My%20Cutscene))
      (Variables|Default|SetSkipped%20My%20Cutscene true)
      (CallFunction|UnlockChest)
      (bind _my_key_unlocker (Variables|Default|GetMy%20Key%20Unlocker)
        (:then
          (Actor|DestroyActor _my_key_unlocker))
        (:else)))))

(event Input|KeyboardEvents|SpaceBar
  (params (Key :type Key%20Structure :default "None"))
  (:Pressed
    (Development|PrintString "locked chest input")
    (if (not (Variables|Default|GetSkipped%20My%20Cutscene))
      (Variables|Default|SetSkipped%20My%20Cutscene true)
      (CallFunction|UnlockChest)
      (bind _my_key_unlocker (Variables|Default|GetMy%20Key%20Unlocker)
        (:then
          (Actor|DestroyActor _my_key_unlocker))
        (:else)))))

(event Input|MouseEvents|LeftMouseButton
  (params (Key :type Key%20Structure :default "None"))
  (:Pressed
    (Development|PrintString "locked chest input")
    (if (not (Variables|Default|GetSkipped%20My%20Cutscene))
      (Variables|Default|SetSkipped%20My%20Cutscene true)
      (CallFunction|UnlockChest)
      (bind _my_key_unlocker (Variables|Default|GetMy%20Key%20Unlocker)
        (:then
          (Actor|DestroyActor _my_key_unlocker))
        (:else)))))

(fn ConstructionScript
  (|CallParentFunction))

(fn UnlockChest
  (Variables|Default|SetContainer%20Unlocked true)
  ;[0.207 0.03193 0.5573 1 12] qtderg contribution
  ;
  ; This let's people make a chest openable only by a key by ticking "Invincible" box on instance of Locked Chest blueprint
  (Variables|/Game/SpyroContent/Global_Assets/Global_Components/Damageable_Com.Damageable_Com_C|SetInvincible (Variables|Default|GetDamageable) false)
  (Default|DealDamage (Variables|Default|GetDamageable) "NewEnumerator0" "0, 0, 0" true 0 false))