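; Collectible key actor, filed with the Locked Chest items, that the player picks up by touch.
; On overlap it hides with effects, joins the player's collected-keys list and raises the HUD count, while ResetKey can restore it.
; Shortly after BeginPlay it destroys itself if its object name is among the current save slot's used keys.
; Its mesh and pickup sound follow the saved treasure-skin setting.
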(event OnComponentBeginOverlap(Hitbox)
  (params (OverlappedComponent :type Primitive%20Component%20Object%20Reference) (OtherActor :type Actor%20Object%20Reference) (OtherComp :type Primitive%20Component%20Object%20Reference) (OtherBodyIndex :type Integer) (bFromSweep :type Boolean) (SweepResult :type Hit%20Result%20Structure%20%28by%20ref%29))
  (bind _staticmesh (Variables|Default|GetStaticMesh))
  (bind _returnvalue (Transformation|GetWorldLocation _staticmesh))
  (bind _asbp_base_playable (Utilities|Casting|CastToBP_Base_Playable OtherActor))
  (if (Math|Boolean|ANDBoolean (== (Variables|/Script/Engine.Character|GetCapsuleComponent _asbp_base_playable) OtherComp) (not (Variables|Default|GetCollected)) (Variables|Default|GetSafe%20to%20Collect))
    (Rendering|SetActorHiddenInGame true)
    (Effects|SpawnEmitteratLocation "/Game/SpyroContent/Global_Assets/Global_Level_Items/Gems/Particles/Gem_Star_Burst_Yellow.Gem_Star_Burst_Yellow" _returnvalue)
    (Audio|PlaySoundatLocation (select (Variables|Default|GetS1%20Treasure) "/Game/SpyroContent/Global_Assets/Global_Level_Items/Gems/Audio/gem_collect_s1.gem_collect_s1" "/Game/SpyroContent/Global_Assets/Global_Level_Items/Gems/Audio/gem_collection.gem_collection") _returnvalue "0, 0, 0" 1.0 1.0 0.0 0 0 0)
    (Variables|Default|SetCollected true)
    (Utilities|Array|Add (Variables|/Game/SpyroContent/Global_Assets/Global_Characters/Playable_Characters/BP_Base_Playable.BP_Base_Playable_C|GetMy%20Collected%20Keys _asbp_base_playable) self)
    (bind _foundwidgets (Widget|GetAllWidgetsOfClass "/Game/SpyroContent/Global_Assets/Global_UserInterface/Widgets/HUD.HUD_C" true))
    (Default|SetHUDNumberOfKeys (Utilities|Array|Get(acopy) _foundwidgets) (+ (Variables|/Game/SpyroContent/Global_Assets/Global_UserInterface/Widgets/HUD.HUD_C|GetHUD_NumberOfKeys (Utilities|Array|Get(acopy) _foundwidgets)) 1))
    (Default|ShowKeyHUD (Variables|/Game/SpyroContent/Global_Assets/Global_Characters/Playable_Characters/BP_Base_Playable.BP_Base_Playable_C|GetSpyroContr_Ref _asbp_base_playable))))

(event Custom|Reset%20Key
  (Rendering|SetActorHiddenInGame false)
  (Variables|Default|SetCollected false))

(event Custom|On%20Treasure%20Skin%20Changed
  (CallFunction|SetTreasureSkin))

(event EventBeginPlay
  (CallFunction|SetTreasureSkin)
  (bind _asspyro_persistant_data (Utilities|Casting|CastToSpyro_PersistantData (Game|GetGameInstance)))
  (EventDispatchers|BindEventtoChangeTreasureSkins _asspyro_persistant_data (delegate Custom|On%20Treasure%20Skin%20Changed))
  (Utilities|FlowControl|Delay 1.0)
  (bind _asspyro_persistant_data_2 (Utilities|Casting|CastToSpyro_PersistantData (Game|GetGameInstance)))
  (bind _returnvalue (SaveGame|LoadGamefromSlot (Variables|/Game/SpyroContent/Global_Assets/Global_SaveData/Spyro_PersistantData.Spyro_PersistantData_C|GetCurrent_Level_Name _asspyro_persistant_data_2)))
  (bind _asindividual_level_save_data (Utilities|Casting|CastToIndividual_Level_SaveData _returnvalue))
  (for _array_element (Utilities|Select :Index (Variables|/Game/SpyroContent/Global_Assets/Global_SaveData/Spyro_PersistantData.Spyro_PersistantData_C|GetCurrent_SaveSlot _asspyro_persistant_data_2) :Option%200 (Variables|/Game/SpyroContent/Global_Assets/Global_SaveData/Individual_Level_SaveData.Individual_Level_SaveData_C|GetKeys_Used_0 _asindividual_level_save_data) :Option%201 (Variables|/Game/SpyroContent/Global_Assets/Global_SaveData/Individual_Level_SaveData.Individual_Level_SaveData_C|GetKeys_Used_1 _asindividual_level_save_data) :Option%202 (Variables|/Game/SpyroContent/Global_Assets/Global_SaveData/Individual_Level_SaveData.Individual_Level_SaveData_C|GetKeys_Used_2 _asindividual_level_save_data) :Option%203 (Variables|/Game/SpyroContent/Global_Assets/Global_SaveData/Individual_Level_SaveData.Individual_Level_SaveData_C|GetKeys_Used_3 _asindividual_level_save_data) :Option%204 (Variables|/Game/SpyroContent/Global_Assets/Global_SaveData/Individual_Level_SaveData.Individual_Level_SaveData_C|GetKeys_Used_4 _asindividual_level_save_data) :Option%205 (Variables|/Game/SpyroContent/Global_Assets/Global_SaveData/Individual_Level_SaveData.Individual_Level_SaveData_C|GetKeys_Used_5 _asindividual_level_save_data))
    (if (Utilities|Enum|Equal(Enum) _array_element (Utilities|GetObjectName self))
      (Actor|DestroyActor))))

(fn ConstructionScript)

(fn SetTreasureSkin
  (bind _asspyro_save_data (CallFunction|LoadSpyroGame self))
  (Components|StaticMesh|SetStaticMesh (Variables|Default|GetStaticMesh) (select (Variables|/Game/SpyroContent/Global_Assets/Global_SaveData/Spyro_SaveData.Spyro_SaveData_C|GetS1_Treasure _asspyro_save_data) "/Game/SpyroContent/Global_Assets/Global_Level_Items/Treasure_Containers/Locked_Chest/Static_Meshes/key_s1.key_s1" "/Game/SpyroContent/Global_Assets/Global_Level_Items/Treasure_Containers/Locked_Chest/Static_Meshes/key.key"))
  (Variables|Default|SetS1%20Treasure (Variables|/Game/SpyroContent/Global_Assets/Global_SaveData/Spyro_SaveData.Spyro_SaveData_C|GetS1_Treasure _asspyro_save_data)))