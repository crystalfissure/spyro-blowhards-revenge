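; TNT crate treasure container that explodes on super damage or on hitting a pawn or another container.
; Normal damage lights the fuse and physically launches it along the player's facing, farther on ice, detonating after one second.
; While lit, Tick drags root and drop shadow after the simulated capsule.
; The blast sphere-traces to super-damage Damageable hitboxes and knock players away; item-dropper reset restores the crate.
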(event OnComponentHit(CapsuleComponent)
  (params (HitComponent :type Primitive%20Component%20Object%20Reference) (OtherActor :type Actor%20Object%20Reference) (OtherComp :type Primitive%20Component%20Object%20Reference) (NormalImpulse :type Vector :default "0, 0, 0") (Hit :type Hit%20Result%20Structure%20%28by%20ref%29))
  (Utilities|Casting|CastToPawn OtherActor
    (:then
      _)
    (:CastFailed
      (Utilities|Casting|CastToTreasure_Container_Base_BP OtherActor)))
  (CallFunction|TntBlowsUp))

(event Custom|reset%20tnt%20crate
  (bind _dropshadow (Variables|Default|GetDropshadow))
  (bind _root (Variables|Default|GetRoot))
  (bind _capsule_component (Variables|Default|GetCapsule%20Component))
  (bind _returnvalue (Transformation|GetWorldLocation _root))
  (bind _returnvalue_2 (Transformation|GetWorldLocation _capsule_component))
  (Physics|SetSimulatePhysics (Variables|Default|GetCapsule%20Component) false)
  (CallFunction|ToggleFuse false)
  (Variables|/Game/SpyroContent/Global_Assets/Global_Components/Damageable_Com.Damageable_Com_C|SetInvincible (Variables|Default|GetDamageable) false)
  (Transformation|SetWorldLocation (Variables|Default|GetRoot) (Variables|Default|Getstarting%20location) false false)
  (Transformation|SetWorldLocation (Variables|Default|GetCapsule%20Component) (Math|Vector|MakeVector (.x _returnvalue) (.y _returnvalue) (+ (.z _returnvalue) 41.0)) false false)
  (Transformation|SetWorldLocation _dropshadow (Math|Vector|MakeVector (.x _returnvalue_2) (.y _returnvalue_2) (.z (Transformation|GetWorldLocation _dropshadow))) false false))

(event Custom|tnt%20blows%20up
  (bind _capsule_component (Variables|Default|GetCapsule%20Component))
  (bind _returnvalue (Transformation|GetWorldLocation _capsule_component))
  (if (not (Variables|Default|GetContainer_Destroyed))
    (Audio|PlaySoundatLocation "/Game/SpyroContent/Global_Assets/Global_Level_Items/Treasure_Containers/TNT_Crate/tnt_explosion.tnt_explosion" (Transformation|GetActorLocation) "0, 0, 0" 1.0 1.0 0.0 0 0 0)
    (Variables|/Game/SpyroContent/Global_Assets/Global_Components/Damageable_Com.Damageable_Com_C|SetInvincible (Variables|Default|GetDamageable) false)
    (|CallParentFunction)
    (CallFunction|ToggleFuse false)
    (Effects|SpawnEmitteratLocation "/Game/SpyroContent/Global_Assets/Global_Level_Items/Superflame/Particles/Superflame_Blast.Superflame_Blast" (Transformation|GetWorldLocation (Variables|Default|GetStaticMesh)) (Math|Rotator|MakeRotator 0.0 0.0 (.yaw (Transformation|GetWorldRotation (Variables|Default|GetStaticMesh)))) "2.000000,2.000000,2.000000")
    (bind _outhits (Collision|MultiSphereTraceForObjects _returnvalue _returnvalue 2e+02 (Utilities|Array|MakeArray "ObjectTypeQuery1" "ObjectTypeQuery2" "ObjectTypeQuery3" "ObjectTypeQuery4" "ObjectTypeQuery8" "ObjectTypeQuery9" "ObjectTypeQuery10") false 0 "None"))
    (for _array_element _outhits
      (Utilities|IsValid (.hitactor _array_element)
        (:Is%20Valid
          (Utilities|IsValid (Actor|GetComponentbyClass (.hitactor _array_element) "/Game/SpyroContent/Global_Assets/Global_Components/Damageable_Com.Damageable_Com_C")
            (:Is%20Valid
              (if (and (.bblockinghit _array_element) (== (Variables|/Game/SpyroContent/Global_Assets/Global_Components/Damageable_Com.Damageable_Com_C|GetObject's%20Hitbox%20Component (Actor|GetComponentbyClass (.hitactor _array_element) "/Game/SpyroContent/Global_Assets/Global_Components/Damageable_Com.Damageable_Com_C")) (.hitcomponent _array_element)))
                (Default|DealDamage (Actor|GetComponentbyClass (.hitactor _array_element) "/Game/SpyroContent/Global_Assets/Global_Components/Damageable_Com.Damageable_Com_C") "NewEnumerator0" (Math|Vector|GetForwardVector (Math|Rotator|FindLookatRotation (Transformation|GetActorLocation) (Transformation|GetWorldLocation (.hitcomponent _array_element)))) true 0 false)
                (bind _asbp_base_playable (Utilities|Casting|CastToBP_Base_Playable (.hitactor _array_element)))
                (Character|LaunchCharacter _asbp_base_playable (* (Math|Vector|GetForwardVector (Math|Rotator|FindLookatRotation (Transformation|GetActorLocation) (Transformation|GetWorldLocation (.hitcomponent _array_element)))) 1e+03) false false)))))))))

(event EventBeginPlay
  (|CallParentFunction)
  (Variables|Default|Setstarting%20location (Transformation|GetActorLocation))
  (EventDispatchers|BindEventtoItemDropperSuccessfullyReset (Variables|Default|GetItem_Drop_Component) (delegate Custom|reset%20tnt%20crate)))

(event EventDealDamagetoTreasureContainer
  (bind _capsule_component (Variables|Default|GetCapsule%20Component))
  (if (Variables|/Game/SpyroContent/Global_Assets/Global_Components/Damageable_Com.Damageable_Com_C|GetDeal%20Damage%20-%20Super%20Damage (Variables|Default|GetDamageable))
    (CallFunction|TntBlowsUp)
    (elif (not (Variables|Default|Getfuse%20lit))
      (Variables|/Game/SpyroContent/Global_Assets/Global_Components/Damageable_Com.Damageable_Com_C|SetInvincible (Variables|Default|GetDamageable) true)
      (Variables|/Script/Engine.SceneComponent|SetbAbsoluteLocation (Variables|Default|GetCapsule%20Component) true)
      (CallFunction|ToggleFuse true)
      (Physics|SetSimulatePhysics _capsule_component true)
      (Physics|AddImpulse _capsule_component (* (* (Transformation|GetActorForwardVector (Game|GetPlayerCharacter 0)) 6.5e+02) (select (Variables|Default|Geton%20ice) 1.5 1.0)) "None" true)
      (Utilities|FlowControl|Delay 1.0)
      (if (Variables|Default|Getfuse%20lit)
        (CallFunction|TntBlowsUp)))))

(event EventTick
  (params (DeltaSeconds :type Float%20%28single-precision%29))
  (bind _dropshadow (Variables|Default|GetDropshadow))
  (bind _capsule_component (Variables|Default|GetCapsule%20Component))
  (bind _capsule_component_2 (Variables|Default|GetCapsule%20Component))
  (bind _returnvalue (Transformation|GetWorldLocation _capsule_component))
  (bind _returnvalue_2 (Transformation|GetWorldLocation _capsule_component_2))
  (if (Variables|Default|Getfuse%20lit)
    (Transformation|SetWorldLocation (Variables|Default|GetRoot) (Math|Vector|MakeVector (.x _returnvalue_2) (.y _returnvalue_2) (- (.z _returnvalue_2) 41.0)) false false)
    (Transformation|SetWorldLocation _dropshadow (Math|Vector|MakeVector (.x _returnvalue) (.y _returnvalue) (.z (Transformation|GetWorldLocation _dropshadow))) false false)))

(fn ConstructionScript
  (|CallParentFunction))

(fn ToggleFuse
  (params (fuse%20lit :type Boolean))
  (Variables|Default|Setfuse%20lit fuse%20lit)
  (Components|Activation|SetActive (Variables|Default|GetParticleSystem) fuse%20lit false)
  (Components|Activation|SetActive (Variables|Default|GetFuse_Audio) fuse%20lit false))