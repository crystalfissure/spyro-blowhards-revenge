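; Strong chest treasure container that gives audio feedback when hit by damage it resists.
; On BeginPlay it registers its static mesh as the Damageable component's metal-material part and binds to that component's resisted-damage event.
; Resisted hits play a bump sound at the chest unless S1Mode is set, throttled by a DoOnce that resets after a short delay.
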(event Custom|When%20Damage%20is%20Attempted
  (Utilities|FlowControl|DoOnce false :!label _label
    (:Completed
      (if (Variables|Default|GetS1_Mode)
        _
        (else
          (Audio|PlaySoundatLocation "/Game/SpyroContent/Global_Assets/Global_Level_Items/Treasure_Containers/Strong_Chest/strong_chest_bump.strong_chest_bump" (Transformation|GetActorLocation) "0, 0, 0" 1.0 1.0 0.0 0 0 0)))
      (Utilities|FlowControl|Delay 1.0)
      (goto _label Reset))))

(event EventBeginPlay
  (bind _damageable (Variables|Default|GetDamageable))
  (|CallParentFunction)
  (Variables|/Game/SpyroContent/Global_Assets/Global_Components/Damageable_Com.Damageable_Com_C|SetComponent_with_Metal_Material _damageable (Variables|Default|GetStaticMesh))
  (EventDispatchers|BindEventtoDamageWasAttemptedButI'mResistant _damageable (delegate Custom|When%20Damage%20is%20Attempted)))

(fn ConstructionScript
  (|CallParentFunction))