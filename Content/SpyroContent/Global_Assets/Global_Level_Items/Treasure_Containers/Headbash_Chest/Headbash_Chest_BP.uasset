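; Headbash Chest treasure container, built on a parent container Blueprint that it extends with its own hitbox and mesh setup.
; On BeginPlay it gives the Damageable component its hitbox and metal-material mesh, then binds to the successful-damage event.
; Successful damage turns off collision on the mesh and hitbox.
; Resetting the container runs the parent reset, then restores that collision unless the container is flagged as destroyed.
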(event Custom|On%20Headbash%20Chest%20Destroyed
  (Collision|SetCollisionEnabled (Variables|Default|GetStaticMesh) "NoCollision"))

(event EventBeginPlay
  (|CallParentFunction)
  (Variables|/Game/SpyroContent/Global_Assets/Global_Components/Damageable_Com.Damageable_Com_C|SetObject's%20Hitbox%20Component (Variables|Default|GetDamageable) (Variables|Default|GetHeadbash_Chest_Hitbox))
  (Variables|/Game/SpyroContent/Global_Assets/Global_Components/Damageable_Com.Damageable_Com_C|SetComponent_with_Metal_Material (Variables|Default|GetDamageable) (Variables|Default|GetStaticMesh))
  (EventDispatchers|BindEventtoDamageWasSuccessfullyDealt (Variables|Default|GetDamageable) (delegate Custom|On%20Headbash%20Chest%20Destroyed)))

(event EventResetThisContainer
  (|CallParentFunction)
  (if (not (Variables|Default|GetContainer_Destroyed))
    (Collision|SetCollisionEnabled (Variables|Default|GetStaticMesh) "QueryAndPhysics")))

(fn ConstructionScript
  (|CallParentFunction))