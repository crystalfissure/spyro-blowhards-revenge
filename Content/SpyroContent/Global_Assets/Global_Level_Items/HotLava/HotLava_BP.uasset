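; HotLava_BP is a lava hazard that damages the playable character on contact.
; At BeginPlay it copies the Hitbox mesh onto Collision, and Hitbox overlaps trigger BurnThePlayer.
; That function accepts only the player's capsule, skipping one player state and both invincibility flags.
; It switches one environmental state back to another with a yaw-only rotation, resets damage, deals damage through Damageable and calls DealtDamage.
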(event OnComponentBeginOverlap(Hitbox)
  (params (OverlappedComponent :type Primitive%20Component%20Object%20Reference) (OtherActor :type Actor%20Object%20Reference) (OtherComp :type Primitive%20Component%20Object%20Reference) (OtherBodyIndex :type Integer) (bFromSweep :type Boolean) (SweepResult :type Hit%20Result%20Structure%20%28by%20ref%29))
  (CallFunction|BurnthePlayer OtherActor OtherComp))

(event EventBeginPlay
  (Components|StaticMesh|SetStaticMesh (Variables|Default|GetCollision) (Variables|/Script/Engine.StaticMeshComponent|GetStaticMesh (Variables|Default|GetHitbox))))

(fn ConstructionScript)

(fn BurnthePlayer
  (params (Player%20Ref :type Object%20Object%20Reference) (Comp%20Ref :type Object%20Object%20Reference))
  (bind _asbp_base_playable (Utilities|Casting|CastToBP_Base_Playable Player%20Ref))
  (if (Math|Boolean|ANDBoolean (== (Variables|/Script/Engine.Character|GetCapsuleComponent _asbp_base_playable) Comp%20Ref) (not (Utilities|Enum|Equal(Enum) (Variables|/Game/SpyroContent/Global_Assets/Global_Characters/Playable_Characters/BP_Base_Playable.BP_Base_Playable_C|GetPlayer_State _asbp_base_playable) "NewEnumerator11")) (not (Variables|/Game/SpyroContent/Global_Assets/Global_Characters/Playable_Characters/BP_Base_Playable.BP_Base_Playable_C|GetCHEAT_Invincibility _asbp_base_playable)) (not (Variables|/Game/SpyroContent/Global_Assets/Global_Characters/Playable_Characters/BP_Base_Playable.BP_Base_Playable_C|GetSuperinvincibility _asbp_base_playable)))
    (if (Utilities|Enum|Equal(Enum) (Variables|/Game/SpyroContent/Global_Assets/Global_Characters/Playable_Characters/BP_Base_Playable.BP_Base_Playable_C|GetEnvironmental_State _asbp_base_playable) "NewEnumerator1")
      (Variables|/Game/SpyroContent/Global_Assets/Global_Characters/Playable_Characters/BP_Base_Playable.BP_Base_Playable_C|SetEnvironmental_State _asbp_base_playable "NewEnumerator0")
      (Transformation|SetActorRotation _asbp_base_playable (Math|Rotator|MakeRotator 0.0 0.0 (.yaw (Transformation|GetActorRotation _asbp_base_playable)))))
    (Default|ResetDamage _asbp_base_playable)
    (Default|DealDamage (Variables|/Game/SpyroContent/Global_Assets/Global_Characters/Playable_Characters/BP_Base_Playable.BP_Base_Playable_C|GetDamageable _asbp_base_playable) "NewEnumerator1" "0, 0, 0" false self false)
    (Default|CallDealtDamage)))