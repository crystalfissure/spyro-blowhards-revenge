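; Banana plant teleporter that swallows an overlapping player and spits them out at the linked GoesTo plant.
; On overlap it ends the player's power-up, closes both plants, disables input and hides the player.
; A delayed sequence fades the camera, moves the player, then reopens both plants and restores control.
; Open/close helpers drive the anim Blueprint, pop sound and mesh collision; an incoming-player flag blocks re-triggering at the destination.
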(event OnComponentBeginOverlap(Box)
  (params (OverlappedComponent :type Primitive%20Component%20Object%20Reference) (OtherActor :type Actor%20Object%20Reference) (OtherComp :type Primitive%20Component%20Object%20Reference) (OtherBodyIndex :type Integer) (bFromSweep :type Boolean) (SweepResult :type Hit%20Result%20Structure%20%28by%20ref%29))
  (bind _staticmesh (Variables|Default|GetStaticMesh))
  (bind _asbp_base_playable (Utilities|Casting|CastToBP_Base_Playable OtherActor))
  (bind _asbanana_plant_abp (Utilities|Casting|CastToBananaPlant_ABP (Components|SkeletalMesh|GetAnimInstance (Variables|Default|GetSkeletalMesh))))
  (if (Math|Boolean|ANDBoolean (not (Variables|/Game/SpyroContent/Global_Assets/Global_Level_Items/Banana_Plant/BananaPlant_ABP.BananaPlant_ABP_C|GetABP_Closed _asbanana_plant_abp)) (== (Variables|/Script/Engine.Character|GetCapsuleComponent _asbp_base_playable) OtherComp) (not (Variables|Default|GetA%20Player%20is%20Going%20to%20Me)))
    (Variables|Default|SetPlayer%20I%20Ate _asbp_base_playable)
    (Default|CallIAteAPlayer)
    (Variables|/Game/SpyroContent/Global_Assets/Global_Characters/Playable_Characters/BP_Base_Playable.BP_Base_Playable_C|SetPowerUp_Time_Remaining _asbp_base_playable 0.0)
    (Collision|SetCollisionEnabled _staticmesh "NoCollision")
    (Collision|SetCollisionResponsetoChannel _staticmesh "ECC_Camera" "ECR_Ignore")
    (bind _goes_to (Variables|Default|GetGoes%20To)
      (:then
        (Collision|SetCollisionEnabled (Variables|BananaPlant_BP_C|GetStaticMesh _goes_to) "NoCollision")
        (Collision|SetCollisionResponsetoChannel (Variables|BananaPlant_BP_C|GetStaticMesh _goes_to) "ECC_Camera" "ECR_Ignore")
        (Variables|BananaPlant_BP_C|SetA%20Player%20is%20Going%20to%20Me _goes_to true))
      (:else
        _))
    (CallFunction|CloseBananaPlant)
    (bind _goes_to_2 (Variables|Default|GetGoes%20To)
      (:then
        (CallFunction|CloseBananaPlant _goes_to_2))
      (:else
        _))
    (CallFunction|DisableThisPlayer'sInputs _asbp_base_playable)
    (Rendering|SetActorHiddenInGame _asbp_base_playable true)
    (bind _current_sunglasses (Variables|/Game/SpyroContent/Global_Assets/Global_Characters/Playable_Characters/BP_Base_Playable.BP_Base_Playable_C|GetCurrent_Sunglasses _asbp_base_playable)
      (:then
        (Rendering|SetActorHiddenInGame _current_sunglasses true))
      (:else
        _))
    (Utilities|FlowControl|Delay 0.5)
    (bind _player_i_ate (Variables|Default|GetPlayer%20I%20Ate)
      (:then
        (bind _spyrocontr_ref (Variables|/Game/SpyroContent/Global_Assets/Global_Characters/Playable_Characters/BP_Base_Playable.BP_Base_Playable_C|GetSpyroContr_Ref _player_i_ate)
          (:then
            (CameraFades|StartCameraFade :self (Game|GetPlayerCameraManager (Variables|/Game/SpyroContent/Global_Assets/Global_Characters/Playable_Characters/Spyro_PlayerController.Spyro_PlayerController_C|GetPlayer_Index_Number _spyrocontr_ref)) :ToAlpha 1.0 :Duration 0.5 :bShouldFadeAudio true :bHoldWhenFinished true))
          (:else
            _)))
      (:else
        _))
    (Utilities|FlowControl|Delay 0.5)
    (bind _player_i_ate_2 (Variables|Default|GetPlayer%20I%20Ate)
      (:then
        (bind _goes_to_3 (Variables|Default|GetGoes%20To)
          (:then
            (Transformation|SetActorRotation _player_i_ate_2 (Transformation|GetActorRotation _goes_to_3))
            (Default|InvokedResetCamera _player_i_ate_2))
          (:else
            _)))
      (:else
        _))
    (Utilities|FlowControl|Delay 0.5)
    (bind _goes_to_4 (Variables|Default|GetGoes%20To)
      (:then
        (bind _player_i_ate_3 (Variables|Default|GetPlayer%20I%20Ate)
          (:then
            (Transformation|SetActorLocationAndRotation _player_i_ate_3 (Math|Vector|MakeVector (.x (.location (Transformation|GetActorTransform _goes_to_4))) (.y (.location (Transformation|GetActorTransform _goes_to_4))) (+ (.z (.location (Transformation|GetActorTransform _goes_to_4))) 5e+01)) (.rotation (Transformation|GetActorTransform _goes_to_4)))
            (bind _spyrocontr_ref_2 (Variables|/Game/SpyroContent/Global_Assets/Global_Characters/Playable_Characters/BP_Base_Playable.BP_Base_Playable_C|GetSpyroContr_Ref _player_i_ate_3)
              (:then
                (CameraFades|StartCameraFade :self (Game|GetPlayerCameraManager (Variables|/Game/SpyroContent/Global_Assets/Global_Characters/Playable_Characters/Spyro_PlayerController.Spyro_PlayerController_C|GetPlayer_Index_Number _spyrocontr_ref_2)) :FromAlpha 1.0 :Duration 0.5 :bShouldFadeAudio true :bHoldWhenFinished true)
                (Utilities|FlowControl|Delay 0.5)
                (bind _goes_to_5 (Variables|Default|GetGoes%20To)
                  (:then
                    (CallFunction|OpenBananaPlant _goes_to_5)
                    (Variables|BananaPlant_BP_C|SetA%20Player%20is%20Going%20to%20Me _goes_to_5 false))
                  (:else
                    _))
                (Utilities|FlowControl|Delay 0.1)
                (bind _player_i_ate_4 (Variables|Default|GetPlayer%20I%20Ate)
                  (:then
                    (Rendering|SetActorHiddenInGame _player_i_ate_4 false)
                    (bind _current_sunglasses_2 (Variables|/Game/SpyroContent/Global_Assets/Global_Characters/Playable_Characters/BP_Base_Playable.BP_Base_Playable_C|GetCurrent_Sunglasses _player_i_ate_4)
                      (:then
                        (Rendering|SetActorHiddenInGame _current_sunglasses_2 false))
                      (:else
                        _))
                    (bind _spyrocontr_ref_3 (Variables|/Game/SpyroContent/Global_Assets/Global_Characters/Playable_Characters/BP_Base_Playable.BP_Base_Playable_C|GetSpyroContr_Ref _player_i_ate_4)
                      (:then
                        (Input|EnableInput _player_i_ate_4 _spyrocontr_ref_3)
                        (Variables|/Game/SpyroContent/Global_Assets/Global_Characters/Playable_Characters/BP_Base_Playable.BP_Base_Playable_C|SetDid%20we%20disable%20input? _player_i_ate_4 false))
                      (:else
                        _)))
                  (:else
                    _))
                (Variables|Default|SetPlayer%20I%20Ate 0)
                (CallFunction|OpenBananaPlant)
                (Collision|SetCollisionResponsetoChannel (Variables|Default|GetStaticMesh) "ECC_Camera" "ECR_Block")
                (bind _goes_to_6 (Variables|Default|GetGoes%20To)
                  (:then
                    (Collision|SetCollisionResponsetoChannel (Variables|BananaPlant_BP_C|GetStaticMesh _goes_to_6) "ECC_Camera" "ECR_Block"))
                  (:else)))
              (:else)))
          (:else)))
      (:else))))

(event EventBeginPlay
  (Collision|SetCollisionEnabled (Variables|Default|GetStaticMesh) "NoCollision"))

(fn ConstructionScript)

(fn CloseBananaPlant
  (Audio|PlaySoundatLocation "/Game/SpyroContent/Global_Assets/Global_Level_Items/Banana_Plant/banana_plant_pop.banana_plant_pop" (Transformation|GetActorLocation) "0, 0, 0" 1.0 1.0 0.0 0 0 0)
  (Collision|SetCollisionEnabled (Variables|Default|GetStaticMesh) "QueryAndPhysics")
  (bind _asbanana_plant_abp (Utilities|Casting|CastToBananaPlant_ABP (Components|SkeletalMesh|GetAnimInstance (Variables|Default|GetSkeletalMesh))))
  (if (not (Variables|/Game/SpyroContent/Global_Assets/Global_Level_Items/Banana_Plant/BananaPlant_ABP.BananaPlant_ABP_C|GetABP_Closed _asbanana_plant_abp))
    (Variables|/Game/SpyroContent/Global_Assets/Global_Level_Items/Banana_Plant/BananaPlant_ABP.BananaPlant_ABP_C|SetABP_Closed _asbanana_plant_abp true)))

(fn OpenBananaPlant
  (Audio|PlaySoundatLocation "/Game/SpyroContent/Global_Assets/Global_Level_Items/Banana_Plant/banana_plant_pop.banana_plant_pop" (Transformation|GetActorLocation) "0, 0, 0" 1.0 1.0 0.0 0 0 0)
  (Collision|SetCollisionEnabled (Variables|Default|GetStaticMesh) "NoCollision")
  (bind _asbanana_plant_abp (Utilities|Casting|CastToBananaPlant_ABP (Components|SkeletalMesh|GetAnimInstance (Variables|Default|GetSkeletalMesh))))
  (if (Variables|/Game/SpyroContent/Global_Assets/Global_Level_Items/Banana_Plant/BananaPlant_ABP.BananaPlant_ABP_C|GetABP_Closed _asbanana_plant_abp)
    (Variables|/Game/SpyroContent/Global_Assets/Global_Level_Items/Banana_Plant/BananaPlant_ABP.BananaPlant_ABP_C|SetABP_Closed _asbanana_plant_abp false)))