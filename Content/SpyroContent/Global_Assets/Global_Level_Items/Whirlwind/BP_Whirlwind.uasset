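; Whirlwind actor that carries an overlapping player from its hitbox up to WhirlwindTop while active.
; Tick centers, lifts and spins the player, then faces them along TargetRotation and nudges them out into a glide for Spyro or a launch for others.
; An optional camera blend follows the ascent, and a countdown timer started near the top forces release.
; Damage or death frees the player; particle heights scale with the top's position.
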(event OnComponentBeginOverlap(Hitbox)
  (params (OverlappedComponent :type Primitive%20Component%20Object%20Reference) (OtherActor :type Actor%20Object%20Reference) (OtherComp :type Primitive%20Component%20Object%20Reference) (OtherBodyIndex :type Integer) (bFromSweep :type Boolean) (SweepResult :type Hit%20Result%20Structure%20%28by%20ref%29))
  (bind _asbp_base_playable (Utilities|Casting|CastToBP_Base_Playable OtherActor))
  (if (Math|Boolean|ANDBoolean (== (Variables|/Script/Engine.Character|GetCapsuleComponent _asbp_base_playable) OtherComp) (not (Utilities|IsValid (Variables|Default|GetCarried_Player))) (not (Utilities|Enum|Equal(Enum) (Variables|/Game/SpyroContent/Global_Assets/Global_Characters/Playable_Characters/BP_Base_Playable.BP_Base_Playable_C|GetPlayer_State _asbp_base_playable) "NewEnumerator11")) (Variables|Default|GetActive))
    (bind _asspyro_persistant_data (Utilities|Casting|CastToSpyro_PersistantData (Game|GetGameInstance)))
    (if (Variables|/Game/SpyroContent/Global_Assets/Global_SaveData/Spyro_PersistantData.Spyro_PersistantData_C|GetReturning_Home _asspyro_persistant_data)
      (Default|EndPortalTransition _asspyro_persistant_data))
    (bind _output_get (Variables|Default|SetCarried_Player _asbp_base_playable))
    (EventDispatchers|BindEventtoPlayerTookDamage _output_get (delegate Custom|Damaged%20in%20Whirlwind))
    (if (Utilities|Enum|Equal(Enum) (Variables|/Game/SpyroContent/Global_Assets/Global_Characters/Playable_Characters/BP_Base_Playable.BP_Base_Playable_C|GetEnvironmental_State _asbp_base_playable) "NewEnumerator1")
      (Variables|/Game/SpyroContent/Global_Assets/Global_Characters/Playable_Characters/BP_Base_Playable.BP_Base_Playable_C|SetEnvironmental_State _asbp_base_playable "NewEnumerator0")
      (Utilities|FlowControl|Delay 0.2)
      (Variables|Default|GetCarried_Player
        (:then
          (bind _player_is_near_top (CallFunction|IsPlayerNearTop? 1e+02 :!label _label))
          (Variables|Default|SetPlayer_Entered_Near_Top _player_is_near_top)
          (Variables|Default|SetFailsafe 1)
          (Utilities|Time|ClearandInvalidateTimerbyHandle (Variables|Default|GetFailsafe_Timer))
          (bind _carried_player (Variables|Default|GetCarried_Player)
            (:then
              (EventDispatchers|BindEventtoAbouttoRespawn _carried_player (delegate Custom|Player%20Died%20in%20Whirlwind))
              (if (Math|Boolean|ANDBoolean (Utilities|Enum|Equal(Enum) (Variables|/Game/SpyroContent/Global_Assets/Global_Characters/Playable_Characters/BP_Base_Playable.BP_Base_Playable_C|GetPlayer_State _carried_player) "NewEnumerator10") (Utilities|Enum|Equal(Enum) (Variables|/Game/SpyroContent/Global_Assets/Global_Components/Damageable_Com.Damageable_Com_C|GetDamage_Being_Taken (Variables|/Game/SpyroContent/Global_Assets/Global_Characters/Playable_Characters/BP_Base_Playable.BP_Base_Playable_C|GetDamageable _carried_player)) "NewEnumerator4") (<= (Variables|/Game/SpyroContent/Global_Assets/Global_Components/Damageable_Com.Damageable_Com_C|GetHit%20Points (Variables|/Game/SpyroContent/Global_Assets/Global_Characters/Playable_Characters/BP_Base_Playable.BP_Base_Playable_C|GetDamageable _carried_player)) 0))
                (Default|ShouldPlayerDie? _carried_player "NewEnumerator0")
                (else
                  (Variables|/Game/SpyroContent/Global_Assets/Global_Characters/Playable_Characters/BP_Base_Playable.BP_Base_Playable_C|SetPlayer_State _carried_player "NewEnumerator9")))
              (Pawn|Components|CharacterMovement|DisableMovement (Variables|/Script/Engine.Character|GetCharacterMovement _carried_player))
              (Variables|Default|SetMoving_Player true)
              (if (and (Variables|Default|GetUse_Whirlwind_Camera) (not (Variables|Default|GetPlayer_Entered_Near_Top)))
                (Variables|/Game/SpyroContent/Global_Assets/Global_Characters/Playable_Characters/BP_Base_Playable.BP_Base_Playable_C|SetCamera_and_Movement_Disabled_by_Whirlwind (Variables|Default|GetCarried_Player) true)
                (Camera|SetFieldOfView (Variables|Default|GetCamera) (Variables|/Script/Engine.CameraComponent|GetFieldOfView (Variables|/Game/SpyroContent/Global_Assets/Global_Characters/Playable_Characters/BP_Base_Playable.BP_Base_Playable_C|GetFollowCamera (Variables|Default|GetCarried_Player))))
                (Game|Player|SetViewTargetwithBlend (Variables|/Game/SpyroContent/Global_Assets/Global_Characters/Playable_Characters/BP_Base_Playable.BP_Base_Playable_C|GetSpyroContr_Ref (Variables|Default|GetCarried_Player)) self 1.0 "VTBlend_Cubic" 0.0 false)))
            (:else
              (Development|PrintString "Carried Player Invalid on Overlap"))))
        (:else
          (Variables|Default|SetMoving_Player false)))
      (else
        (goto _label)))))

(event Custom|Damaged%20in%20Whirlwind
  (Variables|Default|SetMoving_Player false)
  (bind _carried_player (Variables|Default|GetCarried_Player)
    (:then
      (Pawn|Components|CharacterMovement|SetMovementMode (Variables|/Script/Engine.Character|GetCharacterMovement _carried_player) "MOVE_Walking" 0))
    (:else
      _))
  (Variables|Default|SetCarried_Player 0))

(event Custom|Reset%20Forced%20Glide
  (Utilities|FlowControl|DoOnce false) ; enters at Reset
)

(event Custom|Forced%20Glide
  (Utilities|FlowControl|Delay 0.5)
  (Variables|Default|SetMoving_Player false)
  (bind _carried_player (Variables|Default|GetCarried_Player)
    (:then
      (Pawn|Components|CharacterMovement|SetMovementMode (Variables|/Script/Engine.Character|GetCharacterMovement _carried_player) "MOVE_Walking" 0)
      (Utilities|FlowControl|Delay 0.2)
      (bind _asbp_spyro (Utilities|Casting|CastToBP_Spyro _carried_player)
        (:then
          (Variables|/Game/SpyroContent/Global_Assets/Global_Characters/Playable_Characters/BP_Base_Playable.BP_Base_Playable_C|SetPlayer_State _asbp_spyro "NewEnumerator1"))
        (:CastFailed
          (Character|LaunchCharacter _asbp_spyro (* (Math|Vector|GetForwardVector (Variables|Default|GetTargetRotation)) 1e+02) true false)))
      (CallFunction|ResetForcedGlide)
      (Variables|Default|SetCarried_Player 0))
    (:else
      (CallFunction|ResetForcedGlide))))

(event Custom|Player%20Died%20in%20Whirlwind
  (Variables|Default|SetCarried_Player 0)
  (Variables|Default|SetMoving_Player false))

(event EventTick
  (params (DeltaSeconds :type Float%20%28single-precision%29))
  (bind _carried_player (Variables|Default|GetCarried_Player))
  (bind _springarm (Variables|Default|GetSpringArm))
  (bind _returnvalue (Transformation|GetWorldLocation _springarm))
  (bind _capsulecomponent (Variables|/Script/Engine.Character|GetCapsuleComponent _carried_player))
  (if (Variables|Default|GetMoving_Player)
    (bind _carried_player_2 (Variables|Default|GetCarried_Player)
      (:then
        (if (not (Variables|/Game/SpyroContent/Global_Assets/Global_Components/Damageable_Com.Damageable_Com_C|GetFrozen (Variables|/Game/SpyroContent/Global_Assets/Global_Characters/Playable_Characters/BP_Base_Playable.BP_Base_Playable_C|GetDamageable _carried_player_2)))
          (Transformation|SetWorldLocation _springarm (Math|Vector|MakeVector (.x _returnvalue) (.y _returnvalue) (- (.z (Transformation|GetActorLocation (Variables|Default|GetCarried_Player))) 1e+02)) false false)
          (bind _player_is_centered (CallFunction|IsPlayerCentered?))
          (if _player_is_centered
            _
            (else
              (|CenterthePlayer)))
          (bind _player_is_at_the_top (CallFunction|IsPlayeratTop?))
          (bind _player_is_near_top (CallFunction|IsPlayerNearTop? 0.0))
          (if _player_is_near_top
            (Default|WhirlwindCameraExit (Variables|Default|GetCarried_Player)))
          (|ManageFailsafe _player_is_near_top _player_is_at_the_top
            (:then_1
              (if _player_is_at_the_top
                (|FaceForwards)
                (bind _players_facing_forward (CallFunction|IsPlayerFacingForwards? :!label _label))
                (if (or (and _players_facing_forward _player_is_at_the_top) (<= (Variables|Default|GetFailsafe) 0))
                  (Utilities|FlowControl|Sequence
                    (:then_0
                      (Utilities|FlowControl|DoOnce false
                        (:Completed
                          (CallFunction|ForcedGlide))))
                    (:then_1
                      (Transformation|SetWorldLocation _capsulecomponent (+ (Transformation|GetWorldLocation _capsulecomponent) (* (Math|Vector|GetForwardVector _capsulecomponent) (* (Utilities|Time|GetWorldDeltaSeconds) 1e+02))) false false))))
                (else
                  (|PlayerGoesUp)
                  (if (not _player_is_near_top)
                    (|PlayerSpins)
                    (goto _label))))))))
      (:else
        (Variables|Default|SetMoving_Player false)
        (Development|PrintString "Carried Player Invalid, stopped moving player")))))

(event EventBeginPlay
  (bind _whirlwind_top (Variables|Default|GetWhirlwind_Top))
  (bind _whirwind_particles (Variables|Default|GetWhirwind_Particles))
  (bind _relativelocation (Variables|/Script/Engine.SceneComponent|GetRelativeLocation _whirlwind_top))
  (Effects|Components|ParticleSystem|SetFloatParameter _whirwind_particles "Whirlwind Star Height" (* (.z _relativelocation) 0.01))
  (Effects|Components|ParticleSystem|SetFloatParameter _whirwind_particles "Whirlwind Line Height" (* (.z _relativelocation) 1e+01))
  (CallFunction|ToggleWhirlwind (Variables|Default|GetActive)))

(fn ConstructionScript)

(fn IsPlayeratTop?
  (bind _carried_player (Variables|Default|GetCarried_Player)
    (:then
      (return (<= (.z (Transformation|GetWorldLocation (Variables|Default|GetWhirlwind_Top))) (+ (.z (Transformation|GetActorLocation _carried_player)) 5e+01))))
    (:else
      (Development|PrintString "Whirlwind - Is Player at Top - carried player invalid"))))

(fn IsPlayerNearTop?
  (params (Top%20Modifier :type Float%20%28single-precision%29))
  (bind _carried_player (Variables|Default|GetCarried_Player)
    (:then
      (return (<= (- (.z (Transformation|GetWorldLocation (Variables|Default|GetWhirlwind_Top))) (+ (Math|Float|MakeLiteralFloat 8e+01) Top%20Modifier)) (.z (Transformation|GetActorLocation _carried_player)))))
    (:else
      (Development|PrintString "Whirlwind - Is Player Near Top - carried player invalid"))))

(fn IsPlayerFacingForwards?
  (bind _returnvalue (Math|Float|MakeLiteralFloat 15.0))
  (bind _targetrotation (Variables|Default|GetTargetRotation))
  (bind _returnvalue_2 (Transformation|GetWorldRotation _targetrotation))
  (return (Math|Float|InRange(Float) (.yaw (Transformation|GetActorRotation (Variables|Default|GetCarried_Player))) (- (.yaw _returnvalue_2) _returnvalue) (+ (.yaw _returnvalue_2) _returnvalue))))

(fn IsPlayerCentered?
  (bind _returnvalue (Math|Float|MakeLiteralFloat 2e+01))
  (bind _whirlwind_top (Variables|Default|GetWhirlwind_Top))
  (bind _whirlwind_top_2 (Variables|Default|GetWhirlwind_Top))
  (bind _returnvalue_2 (Transformation|GetWorldLocation _whirlwind_top))
  (bind _returnvalue_3 (Transformation|GetWorldLocation _whirlwind_top_2))
  (return (and (Math|Float|InRange(Float) (.x (Transformation|GetActorLocation (Variables|Default|GetCarried_Player))) (+ (.x _returnvalue_3) _returnvalue) (- (.x _returnvalue_3) _returnvalue)) (Math|Float|InRange(Float) (.y (Transformation|GetActorLocation (Variables|Default|GetCarried_Player))) (+ (.y _returnvalue_2) _returnvalue) (- (.y _returnvalue_2) _returnvalue)))))

(fn FailsafeCountdown
  (bind _output_get (Variables|Default|SetFailsafe (- (Variables|Default|GetFailsafe) 1)))
  (if (<= _output_get 0)
    (Utilities|Time|ClearandInvalidateTimerbyHandle (Variables|Default|GetFailsafe_Timer))))

(fn ToggleWhirlwind
  (params (Active :type Boolean))
  (bind _output_get (Variables|Default|SetActive Active))
  (if _output_get
    (Components|Activation|Activate (Variables|Default|GetWhirwind_Particles) false)
    (Audio|Components|Audio|Play (Variables|Default|GetAudio) 0.0)
    (else
      (Components|Activation|Deactivate (Variables|Default|GetWhirwind_Particles))
      (Audio|Components|Audio|Stop (Variables|Default|GetAudio)))))