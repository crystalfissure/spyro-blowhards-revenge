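; Wooden surface level item that swaps a playable character's footstep sounds, and Spyro's charge sound, while the player stands on it.
; Hitbox overlaps with the player's capsule apply the surface's sounds and track the player, then restore class defaults on exit.
; Empty stepped-on and stepped-off functions act as hooks, and debug prints mark each overlap.
; At BeginPlay, the Collision component copies the Hitbox's static mesh.
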(event OnComponentBeginOverlap(Hitbox)
  (params (OverlappedComponent :type Primitive%20Component%20Object%20Reference) (OtherActor :type Actor%20Object%20Reference) (OtherComp :type Primitive%20Component%20Object%20Reference) (OtherBodyIndex :type Integer) (bFromSweep :type Boolean) (SweepResult :type Hit%20Result%20Structure%20%28by%20ref%29))
  (bind _asbp_base_playable (Utilities|Casting|CastToBP_Base_Playable OtherActor))
  (if (== (Variables|/Script/Engine.Character|GetCapsuleComponent _asbp_base_playable) OtherComp)
    (Development|PrintString "STARt OVERLAP")
    (Variables|/Game/SpyroContent/Global_Assets/Global_Characters/Playable_Characters/BP_Base_Playable.BP_Base_Playable_C|SetFootstep_Sound_Even _asbp_base_playable (Variables|Default|GetFootstep%20Sound%20Even))
    (Variables|/Game/SpyroContent/Global_Assets/Global_Characters/Playable_Characters/BP_Base_Playable.BP_Base_Playable_C|SetFootstep_Sound_Odd _asbp_base_playable (Variables|Default|GetFootstep%20Sound%20Odd))
    (Variables|Default|SetPlayer%20on%20me _asbp_base_playable)
    (CallFunction|PlayerSteppedOntoMe)
    (bind _asbp_spyro (Utilities|Casting|CastToBP_Spyro _asbp_base_playable))
    (Variables|/Game/SpyroContent/Global_Assets/Global_Characters/Playable_Characters/Spyro/BP_Spyro.BP_Spyro_C|SetCharge%20Sound _asbp_spyro (Variables|Default|GetCharge%20Sound))))

(event OnComponentEndOverlap(Hitbox)
  (params (OverlappedComponent :type Primitive%20Component%20Object%20Reference) (OtherActor :type Actor%20Object%20Reference) (OtherComp :type Primitive%20Component%20Object%20Reference) (OtherBodyIndex :type Integer))
  (bind _asbp_base_playable (Utilities|Casting|CastToBP_Base_Playable OtherActor))
  (if (== (Variables|/Script/Engine.Character|GetCapsuleComponent _asbp_base_playable) OtherComp)
    (Development|PrintString "end OVERLAP")
    (Variables|/Game/SpyroContent/Global_Assets/Global_Characters/Playable_Characters/BP_Base_Playable.BP_Base_Playable_C|SetFootstep_Sound_Even _asbp_base_playable (.Footstep_Sound_Even (Utilities|GetClassDefaults (Utilities|GetClass _asbp_base_playable))))
    (Variables|/Game/SpyroContent/Global_Assets/Global_Characters/Playable_Characters/BP_Base_Playable.BP_Base_Playable_C|SetFootstep_Sound_Odd _asbp_base_playable (.Footstep_Sound_Odd (Utilities|GetClassDefaults (Utilities|GetClass _asbp_base_playable))))
    (CallFunction|PlayerSteppedOffOfMe)
    (Variables|Default|SetPlayer%20on%20me 0)
    (bind _asbp_spyro (Utilities|Casting|CastToBP_Spyro _asbp_base_playable))
    (Variables|/Game/SpyroContent/Global_Assets/Global_Characters/Playable_Characters/Spyro/BP_Spyro.BP_Spyro_C|SetCharge%20Sound _asbp_spyro (.Charge%20Sound (Utilities|GetClassDefaults (Utilities|GetClass _asbp_spyro))))))

(event EventBeginPlay
  (Components|StaticMesh|SetStaticMesh (Variables|Default|GetCollision) (Variables|/Script/Engine.StaticMeshComponent|GetStaticMesh (Variables|Default|GetHitbox))))

(fn ConstructionScript)

(fn PlayerSteppedOntoMe)

(fn PlayerSteppedOffOfMe)