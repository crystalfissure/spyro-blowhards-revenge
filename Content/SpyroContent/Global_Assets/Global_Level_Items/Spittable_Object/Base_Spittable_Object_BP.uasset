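; Base actor for objects Spyro can swallow, carry hidden in his mouth and spit out.
; Overlap and a looping sphere trace trigger swallowing when state and head-angle checks pass, driving Spyro's AnimBP before attaching to his head.
; Tossing launches it by physics impulse, with an empty SpatIntoDamageable hook, until ground traces return it to swallowable.
; Kill planes and drownable water reset it to its starting transform.
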(event OnComponentBeginOverlap(swallowradius)
  (params (OverlappedComponent :type Primitive%20Component%20Object%20Reference) (OtherActor :type Actor%20Object%20Reference) (OtherComp :type Primitive%20Component%20Object%20Reference) (OtherBodyIndex :type Integer) (bFromSweep :type Boolean) (SweepResult :type Hit%20Result%20Structure%20%28by%20ref%29))
  (CallFunction|PlayerSwallowsMe? OtherActor OtherComp))

(event OnComponentHit(COL)
  (params (HitComponent :type Primitive%20Component%20Object%20Reference) (OtherActor :type Actor%20Object%20Reference) (OtherComp :type Primitive%20Component%20Object%20Reference) (NormalImpulse :type Vector :default "0, 0, 0") (Hit :type Hit%20Result%20Structure%20%28by%20ref%29))
  (Utilities|Casting|CastToBP_Base_Playable OtherActor
    (:CastFailed
      (Utilities|Casting|CastToBP_KillPlane OtherActor
        (:then
          _)
        (:CastFailed
          (Utilities|Casting|CastToDrownable_Water_BP OtherActor
            (:then
              _)
            (:CastFailed
              (Utilities|FlowControl|DoOnce false :!label _label
                (:Completed
                  (Audio|PlaySoundatLocation (Variables|Default|GetHit%20Ground%20SFX) (Transformation|GetActorLocation) "0, 0, 0" 1.0 1.0 0.0 0 0 0)
                  (Utilities|FlowControl|Delay 0.2)
                  (goto _label Reset)))))))
      (CallFunction|ResetSpittableObject))))

(event Custom|Delayed%20Quit%20Lookin%20at%20Me
  (bind _player_swallowing_me (Variables|Default|GetPlayer%20Swallowing%20Me))
  (bind _returnvalue (Transformation|GetActorForwardVector _player_swallowing_me))
  (bind _mesh (Variables|/Script/Engine.Character|GetMesh _player_swallowing_me))
  (bind _returnvalue_2 (Transformation|GetSocketLocation _mesh "Head"))
  (bind _returnvalue_3 (* _returnvalue 5e+01))
  (bind _returnvalue_4 (+ _returnvalue_2 _returnvalue_3))
  (bind _returnvalue_5 (Math|Rotator|FindLookatRotation _returnvalue_2 _returnvalue_4))
  (Utilities|FlowControl|Delay 0.2)
  (Variables|Default|GetPlayer%20Swallowing%20Me
    (:then
      (Default|CallI'veBeenSwallowed)
      (Collision|SetCollisionEnabled (Variables|Default|GetCOL) "NoCollision")
      (Variables|Default|SetSpittable%20Object%20State "NewEnumerator2")
      (Rendering|SetActorHiddenInGame true)
      (bind _asabp_spyro (Utilities|Casting|CastToABP_Spyro (Components|SkeletalMesh|GetAnimInstance (Variables|/Script/Engine.Character|GetMesh (Variables|Default|GetPlayer%20Swallowing%20Me))))
        (:then
          (if (Variables|/Game/SpyroContent/Global_Assets/Global_Characters/Playable_Characters/Spyro/ABPs/ABP_Spyro.ABP_Spyro_C|GetisHoldingItemInMouth _asabp_spyro)
            _
            (else
              (Variables|/Game/SpyroContent/Global_Assets/Global_Characters/Playable_Characters/Spyro/ABPs/ABP_Spyro.ABP_Spyro_C|SetisHoldingItemInMouth _asabp_spyro true)
              (Audio|PlaySoundatLocation "/Game/SpyroContent/Global_Assets/Global_Characters/Playable_Characters/Spyro/Audio/spyro_swallow.spyro_swallow" (Transformation|GetActorLocation) "0, 0, 0" 1.0 1.0 0.0 0 0 0))))
        (:CastFailed
          _))
      (Utilities|FlowControl|Delay 0.3)
      (Utilities|FlowControl|Sequence
        (:then_0
          (bind _player_swallowing_me_2 (Variables|Default|GetPlayer%20Swallowing%20Me)
            (:then
              (bind _asabp_spyro_2 (Utilities|Casting|CastToABP_Spyro (Components|SkeletalMesh|GetAnimInstance (Variables|/Script/Engine.Character|GetMesh _player_swallowing_me_2)))
                (:then
                  (Variables|/Game/SpyroContent/Global_Assets/Global_Characters/Playable_Characters/Spyro/ABPs/ABP_Spyro.ABP_Spyro_C|SetisSwallowing _asabp_spyro_2 false)
                  (Default|LerpSwallowAlpha _player_swallowing_me_2))
                (:CastFailed
                  _))
              (bind _player_swallowing_me_3 (Variables|Default|GetPlayer%20Swallowing%20Me)
                (:then
                  (bind _lookat_target (Variables|/Game/SpyroContent/Global_Assets/Global_Characters/Playable_Characters/BP_Base_Playable.BP_Base_Playable_C|GetLookAt_Target _player_swallowing_me_3)
                    (:then
                      (if (== _lookat_target (Variables|Default|GetCOL))
                        (Variables|/Game/SpyroContent/Global_Assets/Global_Characters/Playable_Characters/BP_Base_Playable.BP_Base_Playable_C|SetLookAt_Target _player_swallowing_me_3 0)
                        (Variables|/Game/SpyroContent/Global_Assets/Global_Characters/Playable_Characters/Spyro/BP_Spyro.BP_Spyro_C|GetObject%20in%20Mouth _player_swallowing_me
                          (:then
                            (bind _asabp_spyro_3 (Utilities|Casting|CastToABP_Spyro (Components|SkeletalMesh|GetAnimInstance _mesh)))
                            (Default|MakeHeadRotator _asabp_spyro_3 (.roll _returnvalue_5) (.pitch _returnvalue_5) (.yaw _returnvalue_5)))
                          (:else))))
                    (:else)))
                (:else)))
            (:else)))
        (:then_1
          (Utilities|FlowControl|Delay 0.2)
          (bind _player_swallowing_me_4 (Variables|Default|GetPlayer%20Swallowing%20Me)
            (:then
              (Transformation|AttachActorToActor _player_swallowing_me_4 "Head" "SnapToTarget" "SnapToTarget" "SnapToTarget" false)
              (Variables|Default|SetSpittable%20Object%20State "NewEnumerator3"))
            (:else)))))
    (:else)))

(event Custom|delayed%20idle%20state
  (Utilities|FlowControl|Delay (select (Variables|Default|GetHeavy) 0.0 0.5))
  (if (Utilities|Enum|Equal(Enum) (Variables|Default|GetSpittable%20Object%20State) "NewEnumerator4")
    (CallFunction|GotoIdleSwallowableState false)
    (if (Variables|Default|GetHeavy)
      (Audio|PlaySoundatLocation "/Game/SpyroContent/Global_Assets/Global_Level_Items/Spittable_Object/Adamantine_Orb/MetalHit2.MetalHit2" (Transformation|GetActorLocation) "0, 0, 0" 1.0 1.0 0.0 0 0 0))))

(event Custom|Wait%20then%20become%20swallowable
  (Utilities|FlowControl|Delay 0.5)
  (CallFunction|GotoIdleSwallowableState true))

(event EventBeginPlay
  (Utilities|Time|SetTimerbyFunctionName 0 "Swallow Ping" 0.2 true)
  (Variables|Default|SetStarting%20Transform (Transformation|GetActorTransform))
  (Utilities|Time|SetTimerbyFunctionName 0 "check for drownable water" 0.5 true)
  (bind _childactor (Variables|/Script/Engine.ChildActorComponent|GetChildActor (Variables|Default|GetDropShadow))
    (:then
      (bind _asdropshadow_bp (Utilities|Casting|CastToDropshadow_BP _childactor))
      (Variables|/Game/SpyroContent/Global_Assets/Global_Level_Items/Dropshadow/Dropshadow_BP.Dropshadow_BP_C|SetOwning%20Component _asdropshadow_bp (Variables|Default|GetCOL)))
    (:else)))

(event EventEndPlay
  (params (EndPlayReason :type EEndPlayReason%20Enum :default "Destroyed"))
  (CallFunction|LeaveSpyro'sMouth))

(event EventTick
  (params (DeltaSeconds :type Float%20%28single-precision%29))
  (bind _player_swallowing_me (Variables|Default|GetPlayer%20Swallowing%20Me))
  (bind _returnvalue (Transformation|GetActorForwardVector _player_swallowing_me))
  (bind _mesh (Variables|/Script/Engine.Character|GetMesh _player_swallowing_me))
  (bind _returnvalue_2 (Transformation|GetSocketLocation _mesh "Head"))
  (bind _returnvalue_3 (* _returnvalue 5e+01))
  (bind _returnvalue_4 (+ _returnvalue_2 _returnvalue_3))
  (bind _returnvalue_5 (Math|Rotator|FindLookatRotation _returnvalue_2 _returnvalue_4))
  (|ManageBeingSpat
    (:then_1
      (bind _player_swallowing_me_2 (Variables|Default|GetPlayer%20Swallowing%20Me)
        (:then
          (if (Utilities|Enum|Equal(Enum) (Variables|Default|GetSpittable%20Object%20State) "NewEnumerator2")
            (Transformation|SetActorLocation (Math|Vector|Lerp(Vector) (Transformation|GetActorLocation) (+ (Transformation|GetSocketLocation (Variables|/Script/Engine.Character|GetMesh _player_swallowing_me_2) "Head") (* (Transformation|GetActorForwardVector _player_swallowing_me_2) 5e+01)) (* (Utilities|Time|GetWorldDeltaSeconds) 2e+01)) false false))
          (bind _returnvalue_6 (CallFunction|CanSpyroLookatMeWithoutSnappingHisNeck? _player_swallowing_me_2 0.0))
          (if (not _returnvalue_6)
            (bind _player_swallowing_me_3 (Variables|Default|GetPlayer%20Swallowing%20Me)
              (:then
                (bind _lookat_target (Variables|/Game/SpyroContent/Global_Assets/Global_Characters/Playable_Characters/BP_Base_Playable.BP_Base_Playable_C|GetLookAt_Target _player_swallowing_me_3)
                  (:then
                    (if (== _lookat_target (Variables|Default|GetCOL))
                      (Variables|/Game/SpyroContent/Global_Assets/Global_Characters/Playable_Characters/BP_Base_Playable.BP_Base_Playable_C|SetLookAt_Target _player_swallowing_me_3 0)
                      (Variables|/Game/SpyroContent/Global_Assets/Global_Characters/Playable_Characters/Spyro/BP_Spyro.BP_Spyro_C|GetObject%20in%20Mouth _player_swallowing_me
                        (:then
                          (bind _asabp_spyro (Utilities|Casting|CastToABP_Spyro (Components|SkeletalMesh|GetAnimInstance _mesh)))
                          (Default|MakeHeadRotator _asabp_spyro (.roll _returnvalue_5) (.pitch _returnvalue_5) (.yaw _returnvalue_5)))
                        (:else))))
                  (:else)))
              (:else))))
        (:else)))))

(fn ConstructionScript)

(fn PlayerSwallowsMe?
  (params (other%20actor :type Object%20Object%20Reference) (other%20comp :type Object%20Object%20Reference))
  (bind _asbp_spyro (Utilities|Casting|CastToBP_Spyro other%20actor))
  (if (Math|Boolean|ANDBoolean (== (Variables|/Script/Engine.Character|GetCapsuleComponent _asbp_spyro) other%20comp) (|airconditions _asbp_spyro) (or (Utilities|Enum|Equal(Enum) (Variables|/Game/SpyroContent/Global_Assets/Global_Characters/Playable_Characters/BP_Base_Playable.BP_Base_Playable_C|GetPlayer_State _asbp_spyro) "NewEnumerator0") (Utilities|Enum|Equal(Enum) (Variables|/Game/SpyroContent/Global_Assets/Global_Characters/Playable_Characters/BP_Base_Playable.BP_Base_Playable_C|GetPlayer_State _asbp_spyro) "NewEnumerator13")) (Utilities|Enum|Equal(Enum) (Variables|Default|GetSpittable%20Object%20State) "NewEnumerator0") (not (Variables|/Game/SpyroContent/Global_Assets/Global_Characters/Playable_Characters/BP_Base_Playable.BP_Base_Playable_C|GetDid%20we%20disable%20input? _asbp_spyro)) (not (Variables|Default|GetUnswallowable)))
    (Variables|Default|GetPlayer%20Swallowing%20Me
      (:then)
      (:else
        (Variables|/Game/SpyroContent/Global_Assets/Global_Characters/Playable_Characters/BP_Base_Playable.BP_Base_Playable_C|GetLookAt_Target _asbp_spyro
          (:then)
          (:else
            (Variables|/Game/SpyroContent/Global_Assets/Global_Characters/Playable_Characters/Spyro/BP_Spyro.BP_Spyro_C|GetObject%20in%20Mouth _asbp_spyro
              (:then)
              (:else
                (bind _returnvalue (CallFunction|CanSpyroLookatMeWithoutSnappingHisNeck? _asbp_spyro 0.0))
                (if (and _returnvalue (< (Math|Float|Absolute(Float) (- (.yaw (Transformation|GetActorRotation _asbp_spyro)) (.yaw (Math|Rotator|FindLookatRotation (Transformation|GetActorLocation _asbp_spyro) (Transformation|GetActorLocation))))) 1.6e+02))
                  (Variables|/Game/SpyroContent/Global_Assets/Global_Characters/Playable_Characters/BP_Base_Playable.BP_Base_Playable_C|SetLookAt_Target _asbp_spyro (Variables|Default|GetCOL))
                  (Variables|Default|SetPlayer%20Swallowing%20Me _asbp_spyro)
                  (Variables|/Game/SpyroContent/Global_Assets/Global_Characters/Playable_Characters/Spyro/BP_Spyro.BP_Spyro_C|SetObject%20in%20Mouth _asbp_spyro self)
                  (CallFunction|DelayedQuitLookinatMe)
                  (bind _asabp_spyro (Utilities|Casting|CastToABP_Spyro (Components|SkeletalMesh|GetAnimInstance (Variables|/Script/Engine.Character|GetMesh _asbp_spyro))))
                  (Default|StopLerpingSwallowAlpha _asbp_spyro)
                  (Variables|/Game/SpyroContent/Global_Assets/Global_Characters/Playable_Characters/Spyro/ABPs/ABP_Spyro.ABP_Spyro_C|SetisSwallowing _asabp_spyro true)
                  (Variables|/Game/SpyroContent/Global_Assets/Global_Characters/Playable_Characters/Spyro/ABPs/ABP_Spyro.ABP_Spyro_C|SetSwallowing%20Alpha _asabp_spyro 1.0)
                  (Collision|SetCollisionResponsetoChannel (Variables|Default|GetCOL) "ECC_Camera" "ECR_Ignore")
                  (CallFunction|IWasSwallowed))))))))))

(fn SwallowPing
  (bind _swallow_radius (Variables|Default|Getswallow%20radius))
  (bind _returnvalue (Transformation|GetWorldLocation _swallow_radius))
  (bind _outhits (Collision|MultiSphereTraceForObjects _returnvalue _returnvalue (Variables|/Script/Engine.SphereComponent|GetSphereRadius _swallow_radius) (Utilities|Array|MakeArray "ObjectTypeQuery3" "ObjectTypeQuery9" "ObjectTypeQuery8") false 0 "None"))
  (bind _array_element (Utilities|Array|ForEachLoopwithBreak _outhits :!label _label)
    (:LoopBody
      (bind _asbp_base_playable (Utilities|Casting|CastToBP_Base_Playable (.hitactor _array_element)))
      (CallFunction|PlayerSwallowsMe? _asbp_base_playable (.hitcomponent _array_element))
      (goto _label Break))))

(fn CanSpyroLookatMeWithoutSnappingHisNeck?
  (params (spyro%20%20ref :type BP%20Spyro%20Object%20Reference) (extra%20range :type Float%20%28single-precision%29))
  (bind _returnvalue (Transformation|GetActorForwardVector))
  (bind _col (Variables|Default|GetCOL))
  (bind _mesh (Variables|/Script/Engine.Character|GetMesh spyro%20%20ref))
  (bind _returnvalue_2 (Transformation|GetWorldLocation _col))
  (bind _returnvalue_3 (Transformation|GetSocketLocation _mesh "Head"))
  (bind _returnvalue_4 (Math|Rotator|FindLookatRotation _returnvalue_3 _returnvalue_2))
  (bind _returnvalue_5 (Math|Vector|GetForwardVector _returnvalue_4))
  (bind _returnvalue_6 (- _returnvalue_5 _returnvalue))
  (bind _returnvalue_7 (Math|Vector|VectorLength _returnvalue_6))
  (Utilities|IsValid spyro%20%20ref
    (:Is%20Valid
      (LocalVariables|SetReturn%20Node (< _returnvalue_7 (- (Variables|/Game/SpyroContent/Global_Assets/Global_Characters/Playable_Characters/Spyro/BP_Spyro.BP_Spyro_C|GetMax%20Head%20Rot%20Vector%20Length spyro%20%20ref) extra%20range)))
      (LocalVariables|SetNewLocalVar_0 _returnvalue_7))
    (:Is%20Not%20Valid
      (LocalVariables|SetReturn%20Node false)
      (LocalVariables|SetNewLocalVar_0 0.0)))
  (return (LocalVariables|GetReturn%20Node) (LocalVariables|GetNewLocalVar_0)))

(fn LeaveSpyro'sMouth
  (Transformation|DetachFromActor "KeepWorld" "KeepWorld" "KeepWorld")
  (bind _player_swallowing_me (Variables|Default|GetPlayer%20Swallowing%20Me)
    (:then
      (bind _lookat_target (Variables|/Game/SpyroContent/Global_Assets/Global_Characters/Playable_Characters/BP_Base_Playable.BP_Base_Playable_C|GetLookAt_Target _player_swallowing_me)
        (:then
          (if (== _lookat_target (Variables|Default|GetCOL))
            (Variables|/Game/SpyroContent/Global_Assets/Global_Characters/Playable_Characters/BP_Base_Playable.BP_Base_Playable_C|SetLookAt_Target _player_swallowing_me 0)))
        (:else
          _))
      (Variables|/Game/SpyroContent/Global_Assets/Global_Characters/Playable_Characters/Spyro/BP_Spyro.BP_Spyro_C|SetObject%20in%20Mouth _player_swallowing_me 0)
      (Default|StopLerpingSwallowAlpha _player_swallowing_me)
      (bind _asabp_spyro (Utilities|Casting|CastToABP_Spyro (Components|SkeletalMesh|GetAnimInstance (Variables|/Script/Engine.Character|GetMesh _player_swallowing_me)))
        (:then
          (Variables|/Game/SpyroContent/Global_Assets/Global_Characters/Playable_Characters/Spyro/ABPs/ABP_Spyro.ABP_Spyro_C|SetisHoldingItemInMouth _asabp_spyro false)
          (Variables|/Game/SpyroContent/Global_Assets/Global_Characters/Playable_Characters/Spyro/ABPs/ABP_Spyro.ABP_Spyro_C|SetisSwallowing _asabp_spyro false)
          (Default|DeflateCheeks _player_swallowing_me)
          (Variables|/Game/SpyroContent/Global_Assets/Global_Characters/Playable_Characters/Spyro/ABPs/ABP_Spyro.ABP_Spyro_C|SetSwallowing%20Alpha _asabp_spyro 0.0))
        (:CastFailed
          _))
      (Variables|Default|SetPlayer%20Swallowing%20Me 0))
    (:else)))

(fn ResetSpittableObject
  (bind _starting_transform (Variables|Default|GetStarting%20Transform))
  (CallFunction|GotoIdleSwallowableState true)
  (CallFunction|LeaveSpyro'sMouth)
  (Transformation|SetActorTransform (Variables|Default|GetStarting%20Transform))
  (Effects|SpawnEmitteratLocation "/Game/SpyroContent/Global_Assets/Global_Particles/P_DustCloud.P_DustCloud" (.location _starting_transform))
  (Audio|PlaySoundatLocation "/Game/SpyroContent/Global_Assets/Global_Characters/AI_Characters/death_poof_s1.death_poof_s1" (.location _starting_transform) "0, 0, 0" 1.0 1.0 0.0 0 0 0)
  (Development|PrintString "RESET SPITTABLE OBJECT" true true "(R=0.000000,G=0.660000,B=1.000000,A=1.000000)" 3e+01))

(fn TosstheBall
  (params (Launching%20Forward%20Vector :type Vector))
  (bind _returnvalue (Transformation|GetActorLocation))
  (bind _returnvalue_2 (Transformation|GetActorForwardVector))
  (bind _forward_launch_power (Variables|Default|GetForward%20Launch%20Power))
  (bind _col (Variables|Default|GetCOL))
  (bind _returnvalue_3 (Math|Float|MakeLiteralFloat _forward_launch_power))
  (bind _returnvalue_4 (* Launching%20Forward%20Vector _returnvalue_3))
  (bind _player_swallowing_me (Variables|Default|GetPlayer%20Swallowing%20Me)
    (:then
      (bind _outhit (Collision|LineTraceForObjects (+ _returnvalue (* _returnvalue_2 -5e+01)) (+ _returnvalue (* _returnvalue_2 75.0)) (Utilities|Array|MakeArray "ObjectTypeQuery1" "ObjectTypeQuery2" "ObjectTypeQuery3" "ObjectTypeQuery9" "ObjectTypeQuery8" "ObjectTypeQuery7") false (Utilities|Array|MakeArray (Variables|Default|GetPlayer%20Swallowing%20Me)) "None"))
      (Utilities|IsValid (.hitactor _outhit)
        (:Is%20Valid
          (Utilities|IsValid (Actor|GetComponentbyClass (.hitactor _outhit) "/Game/SpyroContent/Global_Assets/Global_Components/Damageable_Com.Damageable_Com_C")
            (:Is%20Valid
              (CallFunction|SpatIntoDamageable (Actor|GetComponentbyClass (.hitactor _outhit) "/Game/SpyroContent/Global_Assets/Global_Components/Damageable_Com.Damageable_Com_C"))
              (Variables|Default|SetPlayer%20Who%20Last%20Spat%20Me _player_swallowing_me :!label _label)
              (Audio|PlaySoundatLocation "/Game/SpyroContent/Global_Assets/Global_Characters/Playable_Characters/Spyro/Audio/spyro_spit.spyro_spit" (Transformation|GetActorLocation _player_swallowing_me) "0, 0, 0" 1.0 1.0 0.0 0 0 0)
              (Transformation|DetachFromActor _player_swallowing_me "KeepWorld" "KeepWorld" "KeepWorld")
              (Transformation|SetActorLocationAndRotation (select (.bblockinghit _outhit) (+ (Transformation|GetActorLocation _player_swallowing_me) (* (Transformation|GetActorUpVector _player_swallowing_me) 5e+01)) (select (Utilities|Enum|Equal(Enum) (Variables|/Game/SpyroContent/Global_Assets/Global_Characters/Playable_Characters/BP_Base_Playable.BP_Base_Playable_C|GetPlayer_State _player_swallowing_me) "NewEnumerator14") (+ (Transformation|GetWorldLocation (Variables|/Game/SpyroContent/Global_Assets/Global_Characters/Playable_Characters/BP_Base_Playable.BP_Base_Playable_C|GetFollowCamera _player_swallowing_me)) (* (Math|Vector|GetForwardVector (Variables|/Game/SpyroContent/Global_Assets/Global_Characters/Playable_Characters/BP_Base_Playable.BP_Base_Playable_C|GetFollowCamera _player_swallowing_me)) 2e+02)) (+ (Transformation|GetActorLocation _player_swallowing_me) (* (Transformation|GetActorForwardVector _player_swallowing_me) 5e+01)))) (Math|Rotator|MakeRotator 0.0 0.0 (.yaw (Transformation|GetActorRotation _player_swallowing_me))) true)
              (CallFunction|LeaveSpyro'sMouth :!label _label_2)
              (Rendering|SetActorHiddenInGame false)
              (Variables|Default|SetSpittable%20Object%20State "NewEnumerator4")
              (Physics|SetSimulatePhysics _col true)
              (Collision|SetCollisionResponsetoChannel _col "ECC_Camera" "ECR_Ignore")
              (Collision|SetCollisionEnabled _col "QueryAndPhysics")
              (Physics|AddImpulse (Variables|Default|GetCOL) (Math|Vector|MakeVector (.x _returnvalue_4) (.y _returnvalue_4) (+ (.z _returnvalue_4) (Math|Float|MakeLiteralFloat (Variables|Default|GetUpwards%20Launch%20Power)))) "None" true))
            (:Is%20Not%20Valid
              (if (Utilities|Enum|Equal(Enum) (Collision|GetCollisionObjectType (.hitcomponent _outhit)) "ECC_WorldStatic")
                (goto _label)))))
        (:Is%20Not%20Valid
          (goto _label))))
    (:else
      (goto _label_2))))

(fn GotoIdleSwallowableState
  (params (dont%20check%20for%20ground :type Boolean))
  (bind _returnvalue (Transformation|GetActorLocation))
  (bind (_x _y _z) (Math|Vector|BreakVector _returnvalue))
  (if dont%20check%20for%20ground
    (bind _col (Variables|Default|GetCOL :!label _label)
      (:then
        (Physics|SetSimulatePhysics _col false)
        (Variables|Default|SetSpittable%20Object%20State "NewEnumerator0")
        (Rendering|SetActorHiddenInGame false)
        (Collision|SetCollisionEnabled (Variables|Default|GetCOL) "QueryAndPhysics")
        (Collision|SetCollisionResponsetoChannel (Variables|Default|GetCOL) "ECC_Camera" "ECR_Block")
        (Collision|ClearMoveIgnoreActors (Variables|Default|GetCOL))
        (bind _outactors (Actor|GetAllActorsOfClass "/Game/SpyroContent/Global_Assets/Global_Characters/Playable_Characters/BP_Base_Playable.BP_Base_Playable_C"))
        (for _array_element _outactors
          (Collision|IgnoreActorwhenMoving (Variables|/Script/Engine.Character|GetCapsuleComponent _array_element) self false)))
      (:else))
    (else
      (bind _col_2 (Variables|Default|GetCOL)
        (:then
          (bind _outhits (Class|KismetSystemLibrary|LineTraceMultiforObjects _returnvalue (Math|Vector|MakeVector _x _y (- _z (+ (Variables|/Script/Engine.SphereComponent|GetSphereRadius _col_2) 5.0))) (Utilities|Array|MakeArray "ObjectTypeQuery1" "ObjectTypeQuery7") false 0 "None" true))
          (bind _array_element_2 (Utilities|Array|ForEachLoopwithBreak _outhits :!label _label_2)
            (:LoopBody
              (if (.bblockinghit _array_element_2)
                (Utilities|Casting|CastToBase_Enemy_BP (.hitactor _array_element_2)
                  (:CastFailed
                    (Utilities|FlowControl|Sequence
                      (:then_0
                        (goto _label))
                      (:then_1
                        (goto _label_2 Break)))))))))
        (:else)))))

(fn SpatIntoDamageable
  (params (Damageable :type Damageable%20Com%20Object%20Reference)))

(fn IWasSwallowed)

(fn CheckforDrownableWater
  (bind _returnvalue (Transformation|GetActorLocation))
  (bind (_x _y _z) (Math|Vector|BreakVector _returnvalue))
  (bind _outhit (Collision|LineTraceForObjects _returnvalue (Math|Vector|MakeVector _x _y (- _z (+ (* (Variables|/Script/Engine.SphereComponent|GetSphereRadius (Variables|Default|GetCOL)) 2.0) 2e+01))) (Utilities|Array|MakeArray "ObjectTypeQuery1") false 0 "None"))
  (if (.bblockinghit _outhit)
    (Utilities|Casting|CastToDrownable_Water_BP (.hitactor _outhit))
    (switch Utilities|FlowControl|Switch|SwitchonSpittable_Object_States (Variables|Default|GetSpittable%20Object%20State)
      (:NewEnumerator0
        _)
      (:NewEnumerator1
        _)
      (:NewEnumerator4
        _))
    (CallFunction|ResetSpittableObject)))