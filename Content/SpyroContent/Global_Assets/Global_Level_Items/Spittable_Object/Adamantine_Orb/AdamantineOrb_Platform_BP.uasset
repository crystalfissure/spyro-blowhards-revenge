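; Pressure platform that is weighted down by a heavy spittable object, either overlapping its hitbox directly or carried in Spyro's mouth.
; The first valid overlap sets the button's relative location to zero, latches Weighted and fires IWasWeightedDown.
; It also moves the object's starting transform to just above the platform and resets it there, then calls its wait-then-become-swallowable routine.
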(event OnComponentBeginOverlap(Hitbox)
  (params (OverlappedComponent :type Primitive%20Component%20Object%20Reference) (OtherActor :type Actor%20Object%20Reference) (OtherComp :type Primitive%20Component%20Object%20Reference) (OtherBodyIndex :type Integer) (bFromSweep :type Boolean) (SweepResult :type Hit%20Result%20Structure%20%28by%20ref%29))
  (bind _asbase_spittable_object_bp (Utilities|Casting|CastToBase_Spittable_Object_BP OtherActor)
    (:then
      (if (Variables|/Game/SpyroContent/Global_Assets/Global_Level_Items/Spittable_Object/Base_Spittable_Object_BP.Base_Spittable_Object_BP_C|GetHeavy _asbase_spittable_object_bp)
        (CallFunction|PlaceWeightonMe _asbase_spittable_object_bp)))
    (:CastFailed
      (bind _asbp_spyro (Utilities|Casting|CastToBP_Spyro OtherActor))
      (if (== (Variables|/Script/Engine.Character|GetCapsuleComponent _asbp_spyro) OtherComp)
        (bind _object_in_mouth (Variables|/Game/SpyroContent/Global_Assets/Global_Characters/Playable_Characters/Spyro/BP_Spyro.BP_Spyro_C|GetObject%20in%20Mouth _asbp_spyro)
          (:then
            (if (Variables|/Game/SpyroContent/Global_Assets/Global_Level_Items/Spittable_Object/Base_Spittable_Object_BP.Base_Spittable_Object_BP_C|GetHeavy _object_in_mouth)
              (CallFunction|PlaceWeightonMe _object_in_mouth)))
          (:else))))))

(fn ConstructionScript)

(fn PlaceWeightonMe
  (params (Object :type Base%20Spittable%20Object%20BP%20Object%20Reference))
  (bind _returnvalue (Transformation|GetActorLocation))
  (if (not (Variables|Default|Getweighted))
    (Transformation|SetRelativeLocation (Variables|Default|GetButton) "0, 0, 0" false false)
    (Variables|/Game/SpyroContent/Global_Assets/Global_Level_Items/Spittable_Object/Base_Spittable_Object_BP.Base_Spittable_Object_BP_C|SetStarting%20Transform Object (Math|Transform|MakeTransform (Math|Vector|MakeVector (.x _returnvalue) (.y _returnvalue) (+ (.z _returnvalue) 2e+01)) "0, 0, 0" "1,1,1"))
    (Default|ResetSpittableObject Object)
    (Variables|/Game/SpyroContent/Global_Assets/Global_Level_Items/Spittable_Object/Base_Spittable_Object_BP.Base_Spittable_Object_BP_C|SetSpittable%20Object%20State Object "NewEnumerator1")
    (Default|WaitThenBecomeSwallowable Object)
    (Default|CallIWasWeightedDown)
    (Variables|Default|Setweighted true)))