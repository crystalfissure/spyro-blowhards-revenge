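; Adamantine Orb, a spittable object that players swallow and spit to deal super damage to damageable actors.
; Hits, hitbox overlaps in one object state and the parent's spat-into event feed DamageTarget, crediting the last spitter.
; The orb breaks only under super damage of the type it deals, bursting into shards and resetting after a short delay.
; It also resets before player respawns unless a player is swallowing it.
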(event OnComponentHit(COL)
  (params (HitComponent :type Primitive%20Component%20Object%20Reference) (OtherActor :type Actor%20Object%20Reference) (OtherComp :type Primitive%20Component%20Object%20Reference) (NormalImpulse :type Vector :default "0, 0, 0") (Hit :type Hit%20Result%20Structure%20%28by%20ref%29))
  (Utilities|IsValid OtherActor
    (:Is%20Valid
      (if (and (not (== OtherActor (Variables|Default|GetPlayer%20Who%20Last%20Spat%20Me))) (Utilities|Enum|Equal(Enum) (Variables|Default|GetSpittable%20Object%20State) "NewEnumerator4"))
        (CallFunction|DamageTarget? (Actor|GetComponentbyClass OtherActor "/Game/SpyroContent/Global_Assets/Global_Components/Damageable_Com.Damageable_Com_C"))))))

(event OnComponentBeginOverlap(hitbox)
  (params (OverlappedComponent :type Primitive%20Component%20Object%20Reference) (OtherActor :type Actor%20Object%20Reference) (OtherComp :type Primitive%20Component%20Object%20Reference) (OtherBodyIndex :type Integer) (bFromSweep :type Boolean) (SweepResult :type Hit%20Result%20Structure%20%28by%20ref%29))
  (Utilities|IsValid OtherActor
    (:Is%20Valid
      (if (Math|Boolean|ANDBoolean (not (== OtherActor self)) (not (== OtherActor (Variables|Default|GetPlayer%20Who%20Last%20Spat%20Me))) (Utilities|Enum|Equal(Enum) (Variables|Default|GetSpittable%20Object%20State) "NewEnumerator4"))
        (CallFunction|DamageTarget? (Actor|GetComponentbyClass OtherActor "/Game/SpyroContent/Global_Assets/Global_Components/Damageable_Com.Damageable_Com_C"))))))

(event Custom|Damage%20Orb
  (bind _damageable_comp (Variables|Default|GetDamageable_Comp))
  (if (and (Utilities|Enum|Equal(Enum) (Variables|/Game/SpyroContent/Global_Assets/Global_Components/Damageable_Com.Damageable_Com_C|GetDeal%20Damage%20-%20Damage%20Type _damageable_comp) "NewEnumerator4") (Variables|/Game/SpyroContent/Global_Assets/Global_Components/Damageable_Com.Damageable_Com_C|GetDeal%20Damage%20-%20Super%20Damage _damageable_comp))
    (Utilities|FlowControl|DoOnce false :!label _label
      (:Completed
        (Rendering|SetActorHiddenInGame true)
        (Audio|PlaySoundatLocation "/Game/SpyroContent/Global_Assets/Global_Level_Items/Treasure_Containers/Metal_Chest/MetalCrateBreak1.MetalCrateBreak1" (Transformation|GetActorLocation) "0, 0, 0" 1.0 1.0 0.0 0 0 0)
        (Variables|Default|SetSpittable%20Object%20State "NewEnumerator1")
        (Collision|SetCollisionResponsetoChannel (Variables|Default|GetCOL) "ECC_Camera" "ECR_Ignore")
        (bind _returnvalue (Game|SpawnActorfromClass "/Game/SpyroContent/Global_Assets/Global_Level_Items/Treasure_Containers/Basket/Actors/Basket_Burst_BP.Basket_Burst_BP_C" (Transformation|GetActorTransform) "AdjustIfPossibleButAlwaysSpawn" 0 0))
        (Default|ShardBurstAction _returnvalue "/Game/SpyroContent/Global_Assets/Global_Level_Items/Treasure_Containers/Adamantine_Chest/adamantine_shard_1.adamantine_shard_1" "/Game/SpyroContent/Global_Assets/Global_Level_Items/Treasure_Containers/Adamantine_Chest/adamantine_shard_2.adamantine_shard_2")
        (Utilities|FlowControl|Delay 1.0)
        (CallFunction|ResetSpittableObject)
        (goto _label Reset)))))

(event Custom|reset%20when%20any%20player%20dies
  (Variables|Default|GetPlayer%20Swallowing%20Me
    (:then)
    (:else
      (CallFunction|ResetSpittableObject))))

(event EventBeginPlay
  (|CallParentFunction)
  (Variables|/Game/SpyroContent/Global_Assets/Global_Components/Damageable_Com.Damageable_Com_C|SetObject's%20Hitbox%20Component (Variables|Default|GetDamageable_Comp) (Variables|Default|Gethitbox))
  (EventDispatchers|BindEventtoCallDealDamage (Variables|Default|GetDamageable_Comp) (delegate Custom|Damage%20Orb))
  (bind _asspyro_persistant_data (Utilities|Casting|CastToSpyro_PersistantData (Game|GetGameInstance)))
  (EventDispatchers|BindEventtoAnyPlayerIsAbouttoRespawn _asspyro_persistant_data (delegate Custom|reset%20when%20any%20player%20dies)))

(event EventSpatIntoDamageable
  (params (Damageable :type Damageable%20Com%20Object%20Reference))
  (|CallParentFunction Damageable)
  (CallFunction|DamageTarget? Damageable))

(event EventTick
  (params (DeltaSeconds :type Float%20%28single-precision%29))
  (|CallParentFunction DeltaSeconds) ; This node is disabled and will not be called.\nDrag off pins to build functionality.
)

(fn ConstructionScript
  (|CallParentFunction))

(fn DamageTarget?
  (params (damageable :type Damageable%20Com%20Object%20Reference))
  (bind _returnvalue (Transformation|GetActorForwardVector))
  (Utilities|IsValid damageable
    (:Is%20Valid
      (bind _player_who_last_spat_me (Variables|Default|GetPlayer%20Who%20Last%20Spat%20Me)
        (:then
          (Default|DealDamage damageable "NewEnumerator4" _returnvalue true _player_who_last_spat_me false))
        (:else
          (Default|DealDamage damageable "NewEnumerator4" _returnvalue true 0 false))))))