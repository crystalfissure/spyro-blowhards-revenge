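; Spawner actor that spits out spittable LavaRock_BP objects, the first one second after BeginPlay.
; Each rock spawns ahead of the actor, gets its state set and physics enabled, then is launched up and forward by a velocity-change impulse with a spit sound.
; The rock stores a reference to its spawner, and a separate event spawns another rock after a short delay.
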(event Custom|Spawn%20Lava%20Rock
  (bind _returnvalue (Game|SpawnActorfromClass "/Game/SpyroContent/Global_Assets/Global_Level_Items/Spittable_Object/LavaRock/LavaRock_BP.LavaRock_BP_C" (Math|Transform|MakeTransform (+ (.location (Transformation|GetActorTransform)) (* (Transformation|GetActorForwardVector) (Variables|Default|Getforward%20offset))) "0, 0, 0" "1,1,1") "AdjustIfPossibleButAlwaysSpawn" 0 0))
  (Variables|/Game/SpyroContent/Global_Assets/Global_Level_Items/Spittable_Object/Base_Spittable_Object_BP.Base_Spittable_Object_BP_C|SetSpittable%20Object%20State _returnvalue "NewEnumerator1")
  (Physics|SetSimulatePhysics (Variables|/Game/SpyroContent/Global_Assets/Global_Level_Items/Spittable_Object/Base_Spittable_Object_BP.Base_Spittable_Object_BP_C|GetCOL _returnvalue) true)
  (Physics|AddImpulse (Variables|/Game/SpyroContent/Global_Assets/Global_Level_Items/Spittable_Object/Base_Spittable_Object_BP.Base_Spittable_Object_BP_C|GetCOL _returnvalue) (+ (* (Transformation|GetActorUpVector) 5e+02) (* (Transformation|GetActorForwardVector) 2.5e+02)) "None" true)
  (Variables|/Game/SpyroContent/Global_Assets/Global_Level_Items/Spittable_Object/LavaRock/LavaRock_BP.LavaRock_BP_C|SetMy%20Spawner _returnvalue self)
  (Audio|PlaySoundatLocation "/Game/SpyroContent/Global_Assets/Global_Level_Items/Spittable_Object/LavaRock/lava_rock_spit.lava_rock_spit" (Transformation|GetActorLocation) "0, 0, 0" 1.0 1.0 0.0 0 0 0))

(event Custom|Delayed%20spawn%20lava%20rock
  (Utilities|FlowControl|Delay 1.0)
  (CallFunction|SpawnLavaRock))

(event EventBeginPlay
  (Utilities|FlowControl|Delay 1.0)
  (CallFunction|SpawnLavaRock))

(fn ConstructionScript)