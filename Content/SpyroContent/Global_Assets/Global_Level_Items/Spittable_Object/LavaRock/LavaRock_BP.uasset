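; Lava rock spittable object that the player can swallow and spit to damage enemies, containers and other damageable actors.
; When spat, a forward sphere trace from player or camera picks a homing target, and Tick eases only the rock's height toward it.
; Hits, overlaps or proximity deal damage and destroy the rock, spawning debris and impact sound.
; Swallowing or water contact asks its spawner for a replacement; resets and level unloads destroy it.
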(event OnComponentHit(COL)
  (params (HitComponent :type Primitive%20Component%20Object%20Reference) (OtherActor :type Actor%20Object%20Reference) (OtherComp :type Primitive%20Component%20Object%20Reference) (NormalImpulse :type Vector :default "0, 0, 0") (Hit :type Hit%20Result%20Structure%20%28by%20ref%29))
  (bind _returnvalue (Actor|GetComponentbyClass OtherActor "/Game/SpyroContent/Global_Assets/Global_Components/Damageable_Com.Damageable_Com_C"))
  (Utilities|IsValid OtherActor
    (:Is%20Valid
      (switch Utilities|FlowControl|Switch|SwitchonSpittable_Object_States (Variables|Default|GetSpittable%20Object%20State)
        (:NewEnumerator1
          (Utilities|Casting|CastToStaticMeshComponent OtherComp
            (:then
              (Utilities|Casting|CastToTreasure_Container_Base_BP OtherActor
                (:CastFailed
                  (if (< (Math|Vector|VectorLength (Transformation|GetVelocity)) 1e+01)
                    (CallFunction|GotoIdleSwallowableState false)))))
            (:CastFailed
              (Utilities|Casting|CastToPawn OtherActor)
              (Physics|AddImpulse (Variables|Default|GetCOL) "0, 0, 0" "None" true))))
        (:NewEnumerator4
          (if (not (== OtherActor (Variables|Default|GetPlayer%20Who%20Last%20Spat%20Me)))
            (Utilities|IsValid _returnvalue
              (:Is%20Valid
                (CallFunction|DamageTarget _returnvalue))
              (:Is%20Not%20Valid
                (Development|PrintString (Utilities|String|Append (Utilities|GetDisplayName OtherActor) " rock hit something with no damagable comp"))
                (Actor|DestroyActor)))))))))

(event OnComponentBeginOverlap(hitbox)
  (params (OverlappedComponent :type Primitive%20Component%20Object%20Reference) (OtherActor :type Actor%20Object%20Reference) (OtherComp :type Primitive%20Component%20Object%20Reference) (OtherBodyIndex :type Integer) (bFromSweep :type Boolean) (SweepResult :type Hit%20Result%20Structure%20%28by%20ref%29))
  (bind _returnvalue (Actor|GetComponentbyClass OtherActor "/Game/SpyroContent/Global_Assets/Global_Components/Damageable_Com.Damageable_Com_C"))
  (bind _returnvalue_2 (Actor|GetComponentbyClass OtherActor "/Game/SpyroContent/Global_Assets/Global_Components/Child_Components/Walking_AI_Character.Walking_AI_Character_C"))
  (if (and (not (== OtherActor (Variables|Default|GetPlayer%20Who%20Last%20Spat%20Me))) (Utilities|Enum|Equal(Enum) (Variables|Default|GetSpittable%20Object%20State) "NewEnumerator4"))
    (Utilities|IsValid _returnvalue
      (:Is%20Valid
        (Utilities|IsValid _returnvalue_2
          (:Is%20Valid
            (if (not (Utilities|Enum|Equal(Enum) (Variables|/Game/SpyroContent/Global_Assets/Global_Components/Base_AI_Character.Base_AI_Character_C|GetAICharacter_State _returnvalue_2) "NewEnumerator3"))
              (CallFunction|DamageTarget _returnvalue :!label _label)))
          (:Is%20Not%20Valid
            (bind _astreasure_container_base_bp (Utilities|Casting|CastToTreasure_Container_Base_BP OtherActor)
              (:then
                (if (not (Variables|/Game/SpyroContent/Global_Assets/Global_Level_Items/Treasure_Containers/Treasure_Container_Base_BP.Treasure_Container_Base_BP_C|GetContainer_Destroyed _astreasure_container_base_bp))
                  (goto _label)))
              (:CastFailed
                (goto _label)))))))))

(event OnComponentBeginOverlap(COL)
  (params (OverlappedComponent :type Primitive%20Component%20Object%20Reference) (OtherActor :type Actor%20Object%20Reference) (OtherComp :type Primitive%20Component%20Object%20Reference) (OtherBodyIndex :type Integer) (bFromSweep :type Boolean) (SweepResult :type Hit%20Result%20Structure%20%28by%20ref%29))
  (switch Utilities|FlowControl|Switch|SwitchonSpittable_Object_States (Variables|Default|GetSpittable%20Object%20State)
    (:NewEnumerator0
      _)
    (:NewEnumerator1
      _))
  (Utilities|Casting|CastToSwimmable_Water_BP OtherActor)
  (bind _my_spawner (Variables|Default|GetMy%20Spawner)
    (:then
      (Default|SpawnLavaRock _my_spawner))
    (:else
      _))
  (Development|PrintString "rock destroyed by water")
  (Actor|DestroyActor))

(event Custom|clear%20on%20level%20unload
  (Development|PrintString "rock destroyed by level unloaded")
  (Actor|DestroyActor))

(event EventTick
  (params (DeltaSeconds :type Float%20%28single-precision%29))
  (bind _returnvalue (Transformation|GetActorLocation))
  (bind (_x _y) (Math|Vector|BreakVector _returnvalue))
  (|CallParentFunction DeltaSeconds)
  (bind _homing_target (Variables|Default|GetHoming%20Target)
    (:then
      (Transformation|SetActorLocation (Math|Vector|Lerp(Vector) _returnvalue (Math|Vector|MakeVector _x _y (.z (Transformation|GetActorLocation _homing_target))) (* (Utilities|Time|GetWorldDeltaSeconds) 3.5)) false false)
      (if (<= (Transformation|GetDistanceTo (Variables|Default|GetHoming%20Target)) 2e+02)
        (CallFunction|DamageTarget (Actor|GetComponentbyClass (Variables|Default|GetHoming%20Target) "/Game/SpyroContent/Global_Assets/Global_Components/Damageable_Com.Damageable_Com_C"))))
    (:else)))

(event EventBeginPlay
  (|CallParentFunction)
  (bind _asspyro_persistant_data (Utilities|Casting|CastToSpyro_PersistantData (Game|GetGameInstance)))
  (EventDispatchers|BindEventtoUnloadLevel _asspyro_persistant_data (delegate Custom|clear%20on%20level%20unload)))

(event EventDestroyed
  (bind _returnvalue (Transformation|GetActorLocation))
  (|CallParentFunction)
  (Game|SpawnActorfromClass "/Game/SpyroContent/Global_Assets/Global_Level_Items/Spittable_Object/LavaRock/LavaRock_Destructable.LavaRock_Destructable_C" (Math|Transform|MakeTransform _returnvalue "0, 0, 0" "1,1,1") "AdjustIfPossibleButAlwaysSpawn" 0 0)
  (Audio|PlaySoundatLocation "/Game/SpyroContent/Global_Assets/Global_Level_Items/Spittable_Object/LavaRock/lava_rock_impact.lava_rock_impact" _returnvalue "0, 0, 0" 1.0 1.0 0.0 0 0 0))

(fn ConstructionScript
  (|CallParentFunction))

(fn IWasSwallowed
  (|CallParentFunction)
  (bind _my_spawner (Variables|Default|GetMy%20Spawner)
    (:then
      (Default|DelayedSpawnLavaRock _my_spawner))
    (:else)))

(fn DamageTarget
  (params (damag%20comp :type Damageable%20Com%20Object%20Reference))
  (bind _returnvalue (Components|GetOwner damag%20comp))
  (bind _returnvalue_2 (Transformation|GetActorForwardVector))
  (bind _returnvalue_3 (Actor|GetComponentbyClass _returnvalue "/Game/SpyroContent/Global_Assets/Global_Components/Child_Components/Walking_AI_Character.Walking_AI_Character_C"))
  (Utilities|IsValid _returnvalue_3
    (:Is%20Valid
      (if (not (Utilities|Enum|Equal(Enum) (Variables|/Game/SpyroContent/Global_Assets/Global_Components/Base_AI_Character.Base_AI_Character_C|GetAICharacter_State _returnvalue_3) "NewEnumerator3"))
        (bind _player_who_last_spat_me (Variables|Default|GetPlayer%20Who%20Last%20Spat%20Me :!label _label)
          (:then
            (Default|DealDamage damag%20comp "NewEnumerator4" _returnvalue_2 false _player_who_last_spat_me false))
          (:else
            (Default|DealDamage damag%20comp "NewEnumerator4" _returnvalue_2 false 0 false)))
        (Development|PrintString "rock destroyed by damage target" true true "(R=0.000000,G=0.660000,B=1.000000,A=1.000000)" 3e+01)
        (Actor|DestroyActor)))
    (:Is%20Not%20Valid
      (bind _astreasure_container_base_bp (Utilities|Casting|CastToTreasure_Container_Base_BP _returnvalue)
        (:then
          (if (not (Variables|/Game/SpyroContent/Global_Assets/Global_Level_Items/Treasure_Containers/Treasure_Container_Base_BP.Treasure_Container_Base_BP_C|GetContainer_Destroyed _astreasure_container_base_bp))
            (goto _label)))
        (:CastFailed
          (goto _label))))))

(fn TosstheBall
  (params (Launching%20Forward%20Vector :type Vector :default "0, 0, 0"))
  (bind _player_who_last_spat_me (Variables|Default|GetPlayer%20Who%20Last%20Spat%20Me))
  (bind _player_state (Variables|/Game/SpyroContent/Global_Assets/Global_Characters/Playable_Characters/BP_Base_Playable.BP_Base_Playable_C|GetPlayer_State _player_who_last_spat_me))
  (bind _followcamera (Variables|/Game/SpyroContent/Global_Assets/Global_Characters/Playable_Characters/BP_Base_Playable.BP_Base_Playable_C|GetFollowCamera _player_who_last_spat_me))
  (bind _capsulecomponent (Variables|/Script/Engine.Character|GetCapsuleComponent _player_who_last_spat_me))
  (bind _returnvalue (Utilities|Enum|Equal(Enum) _player_state "NewEnumerator14"))
  (bind _returnvalue_2 (select _returnvalue _followcamera _capsulecomponent))
  (|CallParentFunction Launching%20Forward%20Vector)
  (bind _player_who_last_spat_me_2 (Variables|Default|GetPlayer%20Who%20Last%20Spat%20Me)
    (:then
      (bind _outhits (Collision|MultiSphereTraceForObjects (select (Utilities|Enum|Equal(Enum) (Variables|/Game/SpyroContent/Global_Assets/Global_Characters/Playable_Characters/BP_Base_Playable.BP_Base_Playable_C|GetPlayer_State _player_who_last_spat_me_2) "NewEnumerator14") (Transformation|GetWorldLocation (Variables|/Game/SpyroContent/Global_Assets/Global_Characters/Playable_Characters/BP_Base_Playable.BP_Base_Playable_C|GetFollowCamera _player_who_last_spat_me_2)) (Transformation|GetActorLocation _player_who_last_spat_me_2)) (+ (Transformation|GetWorldLocation _returnvalue_2) (* (Math|Vector|GetForwardVector _returnvalue_2) 1.5e+03)) (Variables|/Script/Engine.SphereComponent|GetSphereRadius (Variables|Default|Gethitbox)) (Utilities|Array|MakeArray "ObjectTypeQuery1" "ObjectTypeQuery2" "ObjectTypeQuery3" "ObjectTypeQuery8" "ObjectTypeQuery9" "ObjectTypeQuery10") false 0 "None"))
      (bind _array_element (Utilities|Array|ForEachLoopwithBreak _outhits :!label _label)
        (:LoopBody
          (Utilities|IsValid (.hitactor _array_element)
            (:Is%20Valid
              (if (and (.bblockinghit _array_element) (not (== (.hitactor _array_element) (Variables|Default|GetPlayer%20Who%20Last%20Spat%20Me))))
                (Utilities|IsValid (Actor|GetComponentbyClass (.hitactor _array_element) "/Game/SpyroContent/Global_Assets/Global_Components/Damageable_Com.Damageable_Com_C")
                  (:Is%20Valid
                    (Utilities|IsValid (Actor|GetComponentbyClass (.hitactor _array_element) "/Game/SpyroContent/Global_Assets/Global_Components/Child_Components/Walking_AI_Character.Walking_AI_Character_C")
                      (:Is%20Valid
                        (if (not (Utilities|Enum|Equal(Enum) (Variables|/Game/SpyroContent/Global_Assets/Global_Components/Base_AI_Character.Base_AI_Character_C|GetAICharacter_State (Actor|GetComponentbyClass (.hitactor _array_element) "/Game/SpyroContent/Global_Assets/Global_Components/Child_Components/Walking_AI_Character.Walking_AI_Character_C")) "NewEnumerator3"))
                          (Variables|Default|SetHoming%20Target (.hitactor _array_element) :!label _label_2)
                          (goto _label Break)))
                      (:Is%20Not%20Valid
                        (bind _astreasure_container_base_bp (Utilities|Casting|CastToTreasure_Container_Base_BP (.hitactor _array_element))
                          (:then
                            (if (not (Variables|/Game/SpyroContent/Global_Assets/Global_Level_Items/Treasure_Containers/Treasure_Container_Base_BP.Treasure_Container_Base_BP_C|GetContainer_Destroyed _astreasure_container_base_bp))
                              (goto _label_2)))
                          (:CastFailed
                            (goto _label_2)))))))))))))
    (:else)))

(fn GotoIdleSwallowableState
  (params (dont%20check%20for%20ground :type Boolean))
  (|CallParentFunction dont%20check%20for%20ground)
  (Variables|Default|SetStarting%20Transform (Transformation|GetActorTransform)))

(fn ResetSpittableObject
  (Development|PrintString "rock destroyed by reset spittable object")
  (Actor|DestroyActor))