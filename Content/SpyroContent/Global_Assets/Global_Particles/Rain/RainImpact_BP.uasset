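; Rain impact effect actor that repeatedly repositions itself onto world surfaces around the player camera.
; Each cycle line-traces downward through a randomly offset area around the camera against WorldStatic objects, ignoring kill planes gathered at BeginPlay.
; On a hit, it moves there and a timeline animates its horizontal scale.
; After the animation or a miss, it waits a short random delay and repeats, reusing the same actor.
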(event Custom|Rain%20Impact
  (bind _returnvalue (Game|GetPlayerCameraManager 0))
  (bind _returnvalue_2 (Math|Random|RandomFloatinRange -6e+02 6e+02))
  (bind _returnvalue_3 (Math|Random|RandomFloatinRange -6e+02 6e+02))
  (bind _returnvalue_4 (Camera|GetCameraLocation _returnvalue))
  (bind _returnvalue_5 (+ (.x _returnvalue_4) _returnvalue_2))
  (bind _returnvalue_6 (+ (.y _returnvalue_4) _returnvalue_3))
  (bind _outhit (Collision|LineTraceForObjects (Math|Vector|MakeVector _returnvalue_5 _returnvalue_6 (+ (.z _returnvalue_4) 6e+03)) (Math|Vector|MakeVector _returnvalue_5 _returnvalue_6 (- (.z _returnvalue_4) 6e+03)) (Utilities|Array|MakeArray "ObjectTypeQuery1") false (Variables|Default|GetActors%20to%20Ignore) "None"))
  (if (.bblockinghit _outhit)
    (Transformation|SetActorTransform (Math|Transform|MakeTransform (.location _outhit) "0, 0, 0" "1,1,1"))
    (bind _newtrack_0 (Timeline|Timeline_0 PlayFromStart)
      (:Update
        (Transformation|SetActorScale3D (Math|Vector|MakeVector (select (<= _newtrack_0 0.1) 0.1 _newtrack_0) (select (<= _newtrack_0 0.1) 0.1 _newtrack_0) 1.0)))
      (:Finished
        (Utilities|FlowControl|Delay (Math|Random|RandomFloatinRange 0.0 0.2) :!label _label)
        (CallFunction|RainImpact)))
    (else
      (goto _label))))

(event EventBeginPlay
  (bind _outactors (Actor|GetAllActorsOfClass "/Game/SpyroContent/Global_Assets/Global_Level_Items/BP_KillPlane.BP_KillPlane_C"))
  (Variables|Default|SetActors%20to%20Ignore _outactors)
  (CallFunction|RainImpact))

(event Collision|EventActorBeginOverlap
  (params (OtherActor :type Actor%20Object%20Reference)))

(event EventTick
  (params (DeltaSeconds :type Float%20%28single-precision%29)))

(fn ConstructionScript)