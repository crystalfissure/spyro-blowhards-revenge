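; Headbash_Dust_BP is a short-lived effect actor, apparently for the dust burst of a Spyro headbash.
; On BeginPlay it loops over eight arrow components and spawns the same emitter template at each one's world location and rotation.
; The arrows act as placement markers for the burst.
; A three-second Delay in the loop body does not stall the loop, so all emitters spawn together and the actor destroys itself afterwards.
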(event EventBeginPlay
  (for _array_element (Utilities|Array|MakeArray (Variables|Default|GetArrow) (Variables|Default|GetArrow1) (Variables|Default|GetArrow2) (Variables|Default|GetArrow3) (Variables|Default|GetArrow4) (Variables|Default|GetArrow5) (Variables|Default|GetArrow6) (Variables|Default|GetArrow7))
    (Effects|SpawnEmitteratLocation (Variables|Default|GetEmitter%20Template) (Transformation|GetWorldLocation _array_element) (Transformation|GetWorldRotation _array_element))
    (Utilities|FlowControl|Delay 3.0)
    (Actor|DestroyActor)))

(fn ConstructionScript)