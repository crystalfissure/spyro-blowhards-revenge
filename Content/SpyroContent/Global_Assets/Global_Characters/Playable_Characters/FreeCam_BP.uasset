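; Free-flying camera pawn for photo mode that lets the player fly around while the game is paused.
; setupphotomode stores and replaces the controlled pawn, widens camera view limits, hides the HUD and enables controller full tick during pause.
; Axis inputs move along camera axes and rotate the view, while triggers or polled Q/E keys move vertically.
; Submit or Cancel repossesses the pawn, restores its view limits and HUD, resumes play and destroys the camera.
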(event Custom|set%20up%20photo%20mode
  (params (player%20index :type Integer))
  (bind _returnvalue (Game|GetPlayerController player%20index))
  (bind _playercameramanager (Variables|/Script/Engine.PlayerController|GetPlayerCameraManager _returnvalue))
  (Variables|/Script/Engine.PlayerCameraManager|SetViewYawMax _playercameramanager 1.8e+02)
  (Variables|/Script/Engine.PlayerCameraManager|SetViewYawMin _playercameramanager -179.899994)
  (Variables|/Script/Engine.PlayerCameraManager|SetViewPitchMax _playercameramanager 9e+01)
  (Variables|/Script/Engine.PlayerCameraManager|SetViewPitchMin _playercameramanager -9e+01)
  (Variables|Default|Setcontrolled%20pawn (Pawn|GetControlledPawn _returnvalue))
  (Input|EnableInput _returnvalue)
  (Pawn|Possess _returnvalue self)
  (Game|Player|SetViewTargetwithBlend _returnvalue 0 0.0 "VTBlend_Linear" 0.0 false)
  (Variables|/Script/Engine.PlayerController|SetbShouldPerformFullTickWhenPaused _returnvalue true)
  (bind _foundwidgets (Widget|GetAllWidgetsOfClass "/Game/SpyroContent/Global_Assets/Global_UserInterface/Widgets/HUD.HUD_C" true))
  (Utilities|IsValid (Utilities|Array|Get(acopy) _foundwidgets)
    (:Is%20Valid
      (Widget|SetVisibility (Utilities|Array|Get(acopy) _foundwidgets) "Hidden"))
    (:Is%20Not%20Valid
      _))
  (Variables|/Script/Engine.PlayerController|SetbShowMouseCursor _returnvalue false))

(event EventTick
  (params (DeltaSeconds :type Float%20%28single-precision%29))
  (bind _returnvalue (Game|GetPlayerController 0))
  (bind _returnvalue_2 (* DeltaSeconds 1e+02))
  (Utilities|FlowControl|Sequence
    (:then_0
      (if (Game|Player|IsInputKeyDown _returnvalue "Q")
        (Pawn|Input|AddMovementInput "0, 0,-1.000000" _returnvalue_2 true)))
    (:then_1
      (if (Game|Player|IsInputKeyDown _returnvalue "E")
        (Pawn|Input|AddMovementInput "0, 0,1.000000" _returnvalue_2 true)))))

(event Input|ActionEvents|InputActionUI_Submit
  (params (Key :type Key%20Structure :default "None"))
  (bind _returnvalue (Pawn|GetController))
  (:Pressed
    (Utilities|IsValid _returnvalue
      (:Is%20Valid
        (bind _controlled_pawn (Variables|Default|Getcontrolled%20pawn)
          (:then
            (bind _asplayer_controller (Utilities|Casting|CastToPlayerController _returnvalue)
              (:then
                (Game|Player|SetViewTargetwithBlend _asplayer_controller _controlled_pawn 0.0 "VTBlend_Linear" 0.0 false)
                (Variables|/Script/Engine.PlayerController|SetbShouldPerformFullTickWhenPaused _asplayer_controller false))
              (:CastFailed
                _))
            (Pawn|Possess _returnvalue _controlled_pawn)
            (bind _asbp_base_playable (Utilities|Casting|CastToBP_Base_Playable _controlled_pawn)
              (:then
                (Variables|/Script/Engine.PlayerCameraManager|SetViewYawMax (Variables|/Script/Engine.PlayerController|GetPlayerCameraManager _asplayer_controller) (Variables|/Game/SpyroContent/Global_Assets/Global_Characters/Playable_Characters/BP_Base_Playable.BP_Base_Playable_C|GetDefault_View%20Yaw%20Max _asbp_base_playable))
                (Variables|/Script/Engine.PlayerCameraManager|SetViewYawMin (Variables|/Script/Engine.PlayerController|GetPlayerCameraManager _asplayer_controller) (Variables|/Game/SpyroContent/Global_Assets/Global_Characters/Playable_Characters/BP_Base_Playable.BP_Base_Playable_C|GetDefault_View%20Yaw%20Min _asbp_base_playable))
                (Variables|/Script/Engine.PlayerCameraManager|SetViewPitchMax (Variables|/Script/Engine.PlayerController|GetPlayerCameraManager _asplayer_controller) (Variables|/Game/SpyroContent/Global_Assets/Global_Characters/Playable_Characters/BP_Base_Playable.BP_Base_Playable_C|GetDefault_View%20Pitch%20Max _asbp_base_playable))
                (Variables|/Script/Engine.PlayerCameraManager|SetViewPitchMin (Variables|/Script/Engine.PlayerController|GetPlayerCameraManager _asplayer_controller) (Variables|/Game/SpyroContent/Global_Assets/Global_Characters/Playable_Characters/BP_Base_Playable.BP_Base_Playable_C|GetDefault_View%20Pitch%20Min _asbp_base_playable)))
              (:CastFailed
                _)))
          (:else
            _))
        (bind _foundwidgets (Widget|GetAllWidgetsOfClass "/Game/SpyroContent/Global_Assets/Global_UserInterface/Widgets/HUD.HUD_C" true))
        (Utilities|IsValid (Utilities|Array|Get(acopy) _foundwidgets)
          (:Is%20Valid
            (Widget|SetVisibility (Utilities|Array|Get(acopy) _foundwidgets) "Visible"))
          (:Is%20Not%20Valid
            _))
        (CallFunction|ResumeGame self)
        (Actor|DestroyActor)))))

(event Input|ActionEvents|InputActionUI_Cancel
  (params (Key :type Key%20Structure :default "None"))
  (bind _returnvalue (Pawn|GetController))
  (:Pressed
    (Utilities|IsValid _returnvalue
      (:Is%20Valid
        (bind _controlled_pawn (Variables|Default|Getcontrolled%20pawn)
          (:then
            (bind _asplayer_controller (Utilities|Casting|CastToPlayerController _returnvalue)
              (:then
                (Game|Player|SetViewTargetwithBlend _asplayer_controller _controlled_pawn 0.0 "VTBlend_Linear" 0.0 false)
                (Variables|/Script/Engine.PlayerController|SetbShouldPerformFullTickWhenPaused _asplayer_controller false))
              (:CastFailed
                _))
            (Pawn|Possess _returnvalue _controlled_pawn)
            (bind _asbp_base_playable (Utilities|Casting|CastToBP_Base_Playable _controlled_pawn)
              (:then
                (Variables|/Script/Engine.PlayerCameraManager|SetViewYawMax (Variables|/Script/Engine.PlayerController|GetPlayerCameraManager _asplayer_controller) (Variables|/Game/SpyroContent/Global_Assets/Global_Characters/Playable_Characters/BP_Base_Playable.BP_Base_Playable_C|GetDefault_View%20Yaw%20Max _asbp_base_playable))
                (Variables|/Script/Engine.PlayerCameraManager|SetViewYawMin (Variables|/Script/Engine.PlayerController|GetPlayerCameraManager _asplayer_controller) (Variables|/Game/SpyroContent/Global_Assets/Global_Characters/Playable_Characters/BP_Base_Playable.BP_Base_Playable_C|GetDefault_View%20Yaw%20Min _asbp_base_playable))
                (Variables|/Script/Engine.PlayerCameraManager|SetViewPitchMax (Variables|/Script/Engine.PlayerController|GetPlayerCameraManager _asplayer_controller) (Variables|/Game/SpyroContent/Global_Assets/Global_Characters/Playable_Characters/BP_Base_Playable.BP_Base_Playable_C|GetDefault_View%20Pitch%20Max _asbp_base_playable))
                (Variables|/Script/Engine.PlayerCameraManager|SetViewPitchMin (Variables|/Script/Engine.PlayerController|GetPlayerCameraManager _asplayer_controller) (Variables|/Game/SpyroContent/Global_Assets/Global_Characters/Playable_Characters/BP_Base_Playable.BP_Base_Playable_C|GetDefault_View%20Pitch%20Min _asbp_base_playable)))
              (:CastFailed
                _)))
          (:else
            _))
        (bind _foundwidgets (Widget|GetAllWidgetsOfClass "/Game/SpyroContent/Global_Assets/Global_UserInterface/Widgets/HUD.HUD_C" true))
        (Utilities|IsValid (Utilities|Array|Get(acopy) _foundwidgets)
          (:Is%20Valid
            (Widget|SetVisibility (Utilities|Array|Get(acopy) _foundwidgets) "Visible"))
          (:Is%20Not%20Valid
            _))
        (CallFunction|ResumeGame self)
        (Actor|DestroyActor)))))

(event Input|AxisEvents|InputAxisMoveForward
  (params (AxisValue :type Float%20%28single-precision%29))
  (Pawn|Input|AddMovementInput (Math|Vector|GetForwardVector (Variables|Default|GetCamera)) AxisValue true))

(event Input|AxisEvents|InputAxisMoveRight
  (params (AxisValue :type Float%20%28single-precision%29))
  (Pawn|Input|AddMovementInput (Math|Vector|GetRightVector (Variables|Default|GetCamera)) AxisValue true))

(event Input|AxisEvents|InputAxisTurn
  (params (AxisValue :type Float%20%28single-precision%29))
  (Pawn|Input|AddControllerYawInput (* AxisValue (Utilities|Time|GetWorldDeltaSeconds) (Math|Float|MakeLiteralFloat 6e+01))))

(event Input|AxisEvents|InputAxisLookUp
  (params (AxisValue :type Float%20%28single-precision%29))
  (Pawn|Input|AddControllerPitchInput (* AxisValue (Utilities|Time|GetWorldDeltaSeconds) (Math|Float|MakeLiteralFloat 6e+01))))

(event Input|AxisEvents|InputAxisTurnRate
  (params (AxisValue :type Float%20%28single-precision%29))
  (Pawn|Input|AddControllerYawInput (* AxisValue (Utilities|Time|GetWorldDeltaSeconds) (Math|Float|MakeLiteralFloat 6e+01))))

(event Input|AxisEvents|InputAxisLookUpRate
  (params (AxisValue :type Float%20%28single-precision%29))
  (Pawn|Input|AddControllerPitchInput (* AxisValue (Utilities|Time|GetWorldDeltaSeconds) (Math|Float|MakeLiteralFloat 6e+01))))

(event Input|GamepadEvents|GamepadLeftTriggerAxis
  (params (AxisValue :type Float%20%28single-precision%29))
  (Pawn|Input|AddMovementInput "0, 0,-1.000000" AxisValue true))

(event Input|GamepadEvents|GamepadRightTriggerAxis
  (params (AxisValue :type Float%20%28single-precision%29))
  (Pawn|Input|AddMovementInput "0, 0,1.000000" AxisValue true))

(fn ConstructionScript)