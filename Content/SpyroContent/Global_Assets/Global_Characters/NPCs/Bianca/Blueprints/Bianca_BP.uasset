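; Bianca NPC Blueprint that adds rainbow entrance and exit effects to the parent NPC's talk flow.
; When talking starts, it aims the player's look-at target at the rainbow particles, blends to a rainbow camera and plays the sequence.
; After the talking delay, Bianca appears, with a burst, sound and white fade if that camera exists.
; When talking ends, the camera is destroyed and Bianca either poofs away or gains blocking collision.
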(event Custom|On%20Bianca%20Done%20Talking
  (bind _returnvalue (Transformation|GetActorLocation))
  (bind _capsulecomponent (Variables|Default|GetCapsuleComponent))
  (bind _rainbow_camera (Variables|Default|GetRainbow_Camera)
    (:then
      (bind _childactor (Variables|/Script/Engine.ChildActorComponent|GetChildActor _rainbow_camera)
        (:then
          (Actor|DestroyActor _childactor))
        (:else
          _)))
    (:else
      _))
  (if (Variables|Default|GetPoofs%20After%20Talking)
    (Effects|SpawnEmitteratLocation "/Game/SpyroContent/Global_Assets/Global_Characters/NPCs/Bianca/Particles/Rainbow_Burst.Rainbow_Burst" _returnvalue)
    (Audio|PlaySoundatLocation "/Game/SpyroContent/Global_Assets/Global_Characters/NPCs/Bianca/Audio/bianca_rainbow_boom.bianca_rainbow_boom" _returnvalue "0, 0, 0" 1.0 1.0 0.0 0 0 0)
    (Variables|Default|SetWon't%20Talk true)
    (Rendering|SetActorHiddenInGame true)
    (Utilities|FlowControl|Delay 0.2)
    (Actor|DestroyActor)
    (else
      (Collision|SetCollisionObjectType _capsulecomponent "ECC_Pawn")
      (Collision|SetCollisionResponsetoChannel _capsulecomponent "ECC_Pawn" "ECR_Block")
      (Collision|SetCollisionResponsetoChannel _capsulecomponent "ECC_GameTraceChannel4" "ECR_Block")
      (Collision|SetCollisionResponsetoChannel _capsulecomponent "ECC_GameTraceChannel2" "ECR_Block")
      (Collision|SetCollisionResponsetoChannel _capsulecomponent "ECC_Camera" "ECR_Block"))))

(event EventBeginPlay
  (|CallParentFunction)
  (EventDispatchers|BindEventtoDoneTalking (delegate Custom|On%20Bianca%20Done%20Talking)))

(fn ConstructionScript
  (|CallParentFunction))

(fn OnNPCTalkingStart
  (params (Player%20I%20Am%20Talking%20To :type BP%20Base%20Playable%20Object%20Reference))
  (|CallParentFunction Player%20I%20Am%20Talking%20To)
  (bind _rainbow_particle_emitter (Variables|Default|GetRainbow_Particle_Emitter)
    (:then
      (Variables|/Game/SpyroContent/Global_Assets/Global_Characters/Playable_Characters/BP_Base_Playable.BP_Base_Playable_C|SetLookAt_Target Player%20I%20Am%20Talking%20To (Variables|/Script/Engine.Emitter|GetParticleSystemComponent _rainbow_particle_emitter))
      (bind _asplayer_controller (Utilities|Casting|CastToPlayerController (Pawn|GetController Player%20I%20Am%20Talking%20To)))
      (bind _rainbow_camera (Variables|Default|GetRainbow_Camera)
        (:then
          (Game|Player|SetViewTargetwithBlend _asplayer_controller (Variables|/Script/Engine.ChildActorComponent|GetChildActor _rainbow_camera) 1.0 "VTBlend_Linear" 0.0 false)
          (bind _rainbow_sequence_ref (Variables|Default|GetRainbow%20Sequence%20Ref)
            (:then
              (Sequencer|Player|Play (Variables|/Script/LevelSequence.LevelSequenceActor|GetSequencePlayer _rainbow_sequence_ref) :!class /Script/MovieScene.MovieSceneSequencePlayer)
              (bind _rainbow_particle_emitter_2 (Variables|Default|GetRainbow_Particle_Emitter)
                (:then
                  (Components|Activation|Activate (Variables|/Script/Engine.Emitter|GetParticleSystemComponent _rainbow_particle_emitter_2) false))
                (:else)))
            (:else)))
        (:else)))
    (:else)))

(fn AfterTalkingDelay
  (params (Player%20I%20Am%20Talking%20To :type BP%20Base%20Playable%20Object%20Reference))
  (|CallParentFunction Player%20I%20Am%20Talking%20To)
  (Rendering|SetActorHiddenInGame false)
  (Variables|/Script/Engine.ChildActorComponent|GetChildActor (Variables|Default|GetRainbow_Camera)
    (:then
      (Audio|PlaySoundatLocation "/Game/SpyroContent/Global_Assets/Global_Characters/NPCs/Bianca/Audio/bianca_rainbow_boom.bianca_rainbow_boom" (Transformation|GetActorLocation) "0, 0, 0" 1.0 1.0 0.0 0 0 0)
      (CameraFades|StartCameraFade (Game|GetPlayerCameraManager (Variables|/Game/SpyroContent/Global_Assets/Global_Characters/Playable_Characters/Spyro_PlayerController.Spyro_PlayerController_C|GetPlayer_Index_Number (Variables|/Game/SpyroContent/Global_Assets/Global_Characters/Playable_Characters/BP_Base_Playable.BP_Base_Playable_C|GetSpyroContr_Ref Player%20I%20Am%20Talking%20To))) 1.0 0.0 0.5 "(R=1.000000,G=1.000000,B=1.000000,A=1.000000)" false true)
      (Actor|DestroyActor (Variables|Default|GetRainbow_Particle_Emitter))
      (Effects|SpawnEmitteratLocation "/Game/SpyroContent/Global_Assets/Global_Characters/NPCs/Bianca/Particles/Rainbow_Burst.Rainbow_Burst" (Transformation|GetActorLocation)))
    (:else)))