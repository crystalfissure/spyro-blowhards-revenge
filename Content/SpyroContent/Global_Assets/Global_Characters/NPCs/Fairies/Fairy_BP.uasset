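; Fairy NPC that kisses playable characters who touch her, banking gems if the save setting allows, with variants for breath types and powerups.
; BeginPlay grounds her by line trace, tints material slots by variant, and sets powerup duration from difficulty.
; Non-infinite super fairies also poll with a sphere trace to kiss players whose powerup expired.
; Tick turns her toward the player when kissing or not talking; after conversation she can fly up.
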(event OnComponentBeginOverlap(LookAt_Radius)
  (params (OverlappedComponent :type Primitive%20Component%20Object%20Reference) (OtherActor :type Actor%20Object%20Reference) (OtherComp :type Primitive%20Component%20Object%20Reference) (OtherBodyIndex :type Integer) (bFromSweep :type Boolean) (SweepResult :type Hit%20Result%20Structure%20%28by%20ref%29))
  (bind _asbp_base_playable (Utilities|Casting|CastToBP_Base_Playable OtherActor))
  (if (== (Variables|/Script/Engine.Character|GetCapsuleComponent _asbp_base_playable) OtherComp)
    (Variables|Default|SetLookAt_Target _asbp_base_playable)
    (Development|PrintString "began overlap")))

(event OnComponentEndOverlap(LookAt_Radius)
  (params (OverlappedComponent :type Primitive%20Component%20Object%20Reference) (OtherActor :type Actor%20Object%20Reference) (OtherComp :type Primitive%20Component%20Object%20Reference) (OtherBodyIndex :type Integer))
  (bind _asbp_base_playable (Utilities|Casting|CastToBP_Base_Playable OtherActor))
  (if (and (== (Variables|/Script/Engine.Character|GetCapsuleComponent _asbp_base_playable) OtherComp) (== _asbp_base_playable (Variables|Default|GetLookAt_Target)))
    (Variables|Default|SetLookAt_Target 0)
    (Development|PrintString "ended overlap")))

(event OnComponentBeginOverlap(Kiss_Radius)
  (params (OverlappedComponent :type Primitive%20Component%20Object%20Reference) (OtherActor :type Actor%20Object%20Reference) (OtherComp :type Primitive%20Component%20Object%20Reference) (OtherBodyIndex :type Integer) (bFromSweep :type Boolean) (SweepResult :type Hit%20Result%20Structure%20%28by%20ref%29))
  (CallFunction|Kiss OtherActor OtherComp))

(event Custom|Not%20Talking,%20Fly%20Up
  (bind _returnvalue (Transformation|GetActorLocation))
  (bind _capsulecomponent (Variables|Default|GetCapsuleComponent))
  (bind _returnvalue_2 (Transformation|GetWorldLocation _capsulecomponent))
  (bind (_x _y _z) (Math|Vector|BreakVector _returnvalue_2))
  (if (Variables|Default|GetWon't%20Talk%20A%202nd%20Time)
    (Variables|/Game/SpyroContent/Global_Assets/Global_Components/Damageable_Com.Damageable_Com_C|SetDamage_Being_Taken (Variables|Default|GetNPC_Damageable) "NewEnumerator6")
    (Variables|Default|SetNPC_State "NewEnumerator3")
    (CallFunction|ResetNPCDamage)
    (bind _childactor (Variables|/Script/Engine.ChildActorComponent|GetChildActor (Variables|Default|GetTriangle_to_Talk_Text))
      (:then
        (Actor|DestroyActor _childactor))
      (:else
        _))
    (bind _outhit (Collision|LineTraceForObjects _returnvalue_2 (Math|Vector|MakeVector _x _y (- _z 1e+03)) (Utilities|Array|MakeArray "ObjectTypeQuery1") false 0 "None"))
    (if (.bblockinghit _outhit)
      (Variables|Default|SetFly%20Up%20Z%20Location (+ (.Z (Math|Vector|BreakVector (.location _outhit))) 1.9e+02))
      (bind _newtrack_0 (Timeline|Timeline_0 PlayFromStart)
        (:Update
          (Transformation|SetActorLocation (Math|Vector|MakeVector (.x _returnvalue) (.y _returnvalue) (Math|Float|Lerp (.z _returnvalue) (Variables|Default|GetFly%20Up%20Z%20Location) _newtrack_0)) false false))))))

(event Custom|Set%20My%20Difficulty
  (bind _powerup_duration_medium (Variables|Difficulty|GetPowerup%20Duration%20Medium))
  (bind _powerup_duration_medium_2 (Variables|Difficulty|GetPowerup%20Duration%20Medium))
  (bind _asspyro_universal_save_data (CallFunction|LoadUniversalSave))
  (if (Utilities|Enum|Equal(Enum) (Variables|/Game/SpyroContent/Global_Assets/Global_SaveData/Spyro_Universal_Save_Data.Spyro_Universal_Save_Data_C|GetDifficulty _asspyro_universal_save_data) "NewEnumerator4")
    (bind _asspyro_save_data (CallFunction|LoadSpyroGame self))
    (bind _difficulty (CallFunction|ConvertSkillLevelFloattoEnum (Variables|/Game/SpyroContent/Global_Assets/Global_SaveData/Spyro_SaveData.Spyro_SaveData_C|GetSkill_Level _asspyro_save_data)))
    (Variables|FairyAbilities|SetPowerUp_Duration (Utilities|Select :Index _difficulty :NewEnumerator4 _powerup_duration_medium :NewEnumerator0 (Variables|Difficulty|GetPowerup%20Duration%20Easy) :NewEnumerator1 _powerup_duration_medium :NewEnumerator2 (Variables|Difficulty|GetPowerup%20Duration%20Hard) :NewEnumerator3 (Variables|Difficulty|GetPowerup%20Duration%20Nightmare)))
    (else
      (Variables|FairyAbilities|SetPowerUp_Duration (Utilities|Select :Index (Variables|/Game/SpyroContent/Global_Assets/Global_SaveData/Spyro_Universal_Save_Data.Spyro_Universal_Save_Data_C|GetDifficulty _asspyro_universal_save_data) :NewEnumerator4 _powerup_duration_medium_2 :NewEnumerator0 (Variables|Difficulty|GetPowerup%20Duration%20Easy) :NewEnumerator1 _powerup_duration_medium_2 :NewEnumerator2 (Variables|Difficulty|GetPowerup%20Duration%20Hard) :NewEnumerator3 (Variables|Difficulty|GetPowerup%20Duration%20Nightmare))))))

(event Custom|Kiss
  (params (Other%20Actor :type Actor%20Object%20Reference) (Other%20Component :type Primitive%20Component%20Object%20Reference))
  (bind _npc_damageable (Variables|Default|GetNPC_Damageable))
  (bind _asbp_base_playable (Utilities|Casting|CastToBP_Base_Playable Other%20Actor))
  (bind _persdata_ref (Variables|/Game/SpyroContent/Global_Assets/Global_Characters/Playable_Characters/BP_Base_Playable.BP_Base_Playable_C|GetPersData_Ref _asbp_base_playable)
    (:then
      (if (Math|Boolean|ANDBoolean (== (Variables|/Script/Engine.Character|GetCapsuleComponent _asbp_base_playable) Other%20Component) (not (Variables|/Game/SpyroContent/Global_Assets/Global_Components/Damageable_Com.Damageable_Com_C|GetFrozen _npc_damageable)) (not (Variables|/Game/SpyroContent/Global_Assets/Global_Components/Damageable_Com.Damageable_Com_C|GetParalyzed_by_Fear _npc_damageable)) (not (Variables|/Game/SpyroContent/Global_Assets/Global_SaveData/Spyro_PersistantData.Spyro_PersistantData_C|GetPortal_Transition _persdata_ref)))
        (Utilities|FlowControl|DoOnce false
          (:Completed
            (Variables|Default|SetKiss_Target _asbp_base_playable)
            (bind _asfairy_abp (Utilities|Casting|CastToFairy_ABP (Components|SkeletalMesh|GetAnimInstance (Variables|Character|GetMesh))))
            (if (not (Variables|/Game/SpyroContent/Global_Assets/Global_Characters/NPCs/Fairies/Fairy_ABP.Fairy_ABP_C|GetisKissing _asfairy_abp))
              (Variables|/Game/SpyroContent/Global_Assets/Global_Characters/NPCs/Fairies/Fairy_ABP.Fairy_ABP_C|SetisKissing _asfairy_abp true)
              (Variables|Default|SetKissing true)
              (Variables|/Game/SpyroContent/Global_Assets/Global_Components/Damageable_Com.Damageable_Com_C|SetDamage_Being_Taken (Variables|Default|GetNPC_Damageable) "NewEnumerator6")
              (Variables|Default|SetNPC_State (select (Variables|Default|GetinConversation) "NewEnumerator0" "NewEnumerator3"))
              (CallFunction|ResetNPCDamage)
              (bind _asspyro_player_controller (Utilities|Casting|CastToSpyro_PlayerController (Pawn|GetController (Variables|Default|GetKiss_Target))))
              (Default|ShowBreathHUD _asspyro_player_controller)
              (bind _asspyro_universal_save_data (CallFunction|LoadUniversalSave))
              (if (and (Utilities|Enum|Equal(Enum) (Variables|/Game/SpyroContent/Global_Assets/Global_SaveData/Spyro_Universal_Save_Data.Spyro_Universal_Save_Data_C|GetGem_Behavior _asspyro_universal_save_data) "NewEnumerator1") (not (Variables|/Game/SpyroContent/Global_Assets/Global_Characters/Playable_Characters/BP_Base_Playable.BP_Base_Playable_C|GetRespawning (Variables|Default|GetKiss_Target))))
                (Default|PermanentlyCollectGems _asspyro_player_controller)
                (bind _foundwidgets (Widget|GetAllWidgetsOfClass "/Game/SpyroContent/Global_Assets/Global_UserInterface/Widgets/HUD.HUD_C" true))
                (Utilities|IsValid (Utilities|Array|Get(acopy) _foundwidgets)
                  (:Is%20Valid
                    (Default|SavePermanentGems (Utilities|Array|Get(acopy) _foundwidgets))))))))))
    (:else)))

(event Custom|Can%20Kiss%20Again
  (Utilities|FlowControl|DoOnce false) ; enters at Reset
)

(event Custom|Stop%20Being%20Afraid%20-%20Fairy
  (CallFunction|SetFairyVisuals))

(event EventBeginPlay
  (bind _capsulecomponent (Variables|Default|GetCapsuleComponent))
  (bind _player_position (Variables|Default|GetPlayer_Position))
  (bind _capsulecomponent_2 (Variables|Default|GetCapsuleComponent))
  (bind _returnvalue (Transformation|GetWorldLocation _player_position))
  (bind _returnvalue_2 (Transformation|GetWorldLocation _capsulecomponent))
  (bind _returnvalue_3 (Transformation|GetWorldLocation _capsulecomponent_2))
  (bind (_x _y _z) (Math|Vector|BreakVector _returnvalue_2))
  (|CallParentFunction)
  (Utilities|FlowControl|Sequence
    (:then_0
      (EventDispatchers|BindEventtoCallStopBeingAfraid (Variables|Default|GetNPC_Damageable) (delegate Custom|Stop%20Being%20Afraid%20-%20Fairy))
      (CallFunction|SetFairyVisuals)
      (bind _returnvalue_4 (CallFunction|IsFairySuper?))
      (if (and _returnvalue_4 (not (Variables|FairyAbilities|GetInfinite)))
        (Utilities|Time|SetTimerbyFunctionName 0 "Check for Power Up Targets" 0.5 true))
      (if (Variables|Default|GetUnderwater)
        _
        (else
          (Components|DestroyComponent (Variables|Default|GetBubble_Particle))))
      (bind _returnvalue_5 (CallFunction|IsFairySuper?))
      (if _returnvalue_5
        (Components|Activation|Activate (Variables|Default|Getpowerup_hum) false))
      (bind _outhit (Collision|LineTraceForObjects _returnvalue_2 (Math|Vector|MakeVector _x _y (- _z 1e+03)) (Utilities|Array|MakeArray "ObjectTypeQuery1") false 0 "None"))
      (if (.bblockinghit _outhit)
        (Transformation|SetWorldLocation (Variables|Default|GetDropshadow) (Math|Vector|MakeVector (.X (Math|Vector|BreakVector (.location _outhit))) (.Y (Math|Vector|BreakVector (.location _outhit))) (+ (.Z (Math|Vector|BreakVector (.location _outhit))) 5.0)) false false)
        (Variables|Default|SetRespawn_Location (Math|Vector|MakeVector (.X (Math|Vector|BreakVector (.location _outhit))) (.Y (Math|Vector|BreakVector (.location _outhit))) (+ (.Z (Math|Vector|BreakVector (.location _outhit))) 5e+01)))
        (if (Variables|Default|GetWon't%20Talk)
          (CallFunction|NotTalking,FlyUp)
          (else
            (Transformation|SetActorLocation (Math|Vector|MakeVector (.X (Math|Vector|BreakVector (.location _outhit))) (.Y (Math|Vector|BreakVector (.location _outhit))) (+ (.Z (Math|Vector|BreakVector (.location _outhit))) 87.0)) false false)
            (Transformation|SetWorldLocation (Variables|Default|GetPlayer_Position) (Math|Vector|MakeVector (.x _returnvalue) (.y _returnvalue) (+ (.Z (Math|Vector|BreakVector (.location _outhit))) 34.0)) false false)))
        (else
          (Variables|Default|SetRespawn_Location (Math|Vector|MakeVector (.x _returnvalue_3) (.y _returnvalue_3) (- (.z _returnvalue_3) 2e+02))))))
    (:then_1
      (bind _asspyro_persistant_data (Utilities|Casting|CastToSpyro_PersistantData (Game|GetGameInstance))
        (:then
          (EventDispatchers|BindEventtoDifficultyChanged _asspyro_persistant_data (delegate Custom|Set%20My%20Difficulty)))
        (:CastFailed
          _))
      (CallFunction|SetMyDifficulty))
    (:then_2
      (Utilities|FlowControl|Delay 1.0)
      (Development|SetHiddeninGame (Variables|Default|GetDropshadow) false false))))

(event EventTick
  (params (DeltaSeconds :type Float%20%28single-precision%29))
  (bind _returnvalue (Utilities|Time|GetWorldDeltaSeconds))
  (bind _mesh (Variables|Character|GetMesh))
  (bind _mesh_2 (Variables|Character|GetMesh))
  (bind _mesh_3 (Variables|Character|GetMesh))
  (bind _mesh_4 (Variables|Character|GetMesh))
  (bind _npc_damageable (Variables|Default|GetNPC_Damageable))
  (bind _returnvalue_2 (* _returnvalue 2.0))
  (bind _relativerotation (Variables|/Script/Engine.SceneComponent|GetRelativeRotation _mesh))
  (bind _returnvalue_3 (Math|Rotator|Lerp(Rotator) _relativerotation "0,-90.000000, 0" _returnvalue_2 true))
  (if (and (not (Variables|/Game/SpyroContent/Global_Assets/Global_Components/Damageable_Com.Damageable_Com_C|GetFrozen _npc_damageable)) (not (Variables|/Game/SpyroContent/Global_Assets/Global_Components/Damageable_Com.Damageable_Com_C|GetParalyzed_by_Fear _npc_damageable)))
    (bind _lookat_target (Variables|Default|GetLookAt_Target)
      (:then
        (if (or (Variables|Default|GetKissing) (Variables|Default|GetWon't%20Talk))
          (if (and (not (Math|Rotator|Equal(Rotator) (Transformation|GetWorldRotation _mesh_2) (Math|Rotator|MakeRotator 0.0 0.0 (.yaw (Math|Rotator|Lerp(Rotator) (Transformation|GetWorldRotation _mesh_4) (Math|Rotator|MakeRotator 0.0 0.0 (- (.Yaw (Math|Rotator|BreakRotator (Math|Rotator|FindLookatRotation (Transformation|GetWorldLocation _mesh_4) (Transformation|GetActorLocation _lookat_target)))) 9e+01)) (* (Utilities|Time|GetWorldDeltaSeconds) 4.0) true))) 0.1)) (or (Variables|Default|GetKissing) (Variables|Default|GetWon't%20Talk)))
            (Transformation|SetWorldRotation _mesh_2 (Math|Rotator|MakeRotator 0.0 0.0 (.yaw (Math|Rotator|Lerp(Rotator) (Transformation|GetWorldRotation _mesh_4) (Math|Rotator|MakeRotator 0.0 0.0 (- (.Yaw (Math|Rotator|BreakRotator (Math|Rotator|FindLookatRotation (Transformation|GetWorldLocation _mesh_4) (Transformation|GetActorLocation _lookat_target)))) 9e+01)) (* (Utilities|Time|GetWorldDeltaSeconds) 4.0) true))) false false))
          (else
            (if (not (Math|Rotator|Equal(Rotator) (Variables|/Script/Engine.SceneComponent|GetRelativeRotation _mesh_3) _returnvalue_3 0.1)) :!label _label
              (Transformation|SetRelativeRotation _mesh_3 _returnvalue_3 false false)))))
      (:else
        (goto _label)))))

(event EventDonewithConversation
  (|CallParentFunction)
  (CallFunction|NotTalking,FlyUp))

(fn ConstructionScript
  (|CallParentFunction))

(fn IsFairySuper?
  (bind _is_breath_super_ (CallFunction|UniversalBreathInfo -1 (Variables|FairyAbilities|GetBreath)))
  (return (Math|Boolean|ORBoolean _is_breath_super_ (Variables|FairyAbilities|GetSuperfly) (Variables|FairyAbilities|GetSupercharge) (Variables|FairyAbilities|GetSuperinvincibility))))

(fn SetFairyVisuals
  (bind _supercharge (Variables|FairyAbilities|GetSupercharge))
  (bind _superinvincibility (Variables|FairyAbilities|GetSuperinvincibility))
  (bind _breath (Variables|FairyAbilities|GetBreath))
  (bind _breath_2 (Variables|FairyAbilities|GetBreath))
  (bind _mesh (Variables|Character|GetMesh))
  (bind _supercharge_2 (Variables|FairyAbilities|GetSupercharge))
  (bind _superinvincibility_2 (Variables|FairyAbilities|GetSuperinvincibility))
  (bind _breath_3 (Variables|FairyAbilities|GetBreath))
  (bind _returnvalue (or _supercharge _superinvincibility))
  (bind _returnvalue_2 (or _supercharge_2 _superinvincibility_2))
  (bind _returnvalue_3 (select _returnvalue 1.0 13.0))
  (bind _returnvalue_4 (select _returnvalue_2 "(R=0.260417,G=0.041468,B=0.000000,A=1.000000)" "(R=0.286275,G=0.149689,B=0.000000,A=1.000000)"))
  (bind _returnvalue_5 (Utilities|Select :Index _breath_3 :NewEnumerator20 _returnvalue_3 :NewEnumerator0 13.0 :NewEnumerator1 2.0 :NewEnumerator2 6.0 :NewEnumerator3 6.0 :NewEnumerator4 6.0 :NewEnumerator5 2.0 :NewEnumerator6 1.0 :NewEnumerator7 1.0 :NewEnumerator8 1.0 :NewEnumerator9 1.0 :NewEnumerator10 7.0 :NewEnumerator11 13.0 :NewEnumerator12 1.0 :NewEnumerator13 1.0 :NewEnumerator14 1.0 :NewEnumerator15 6.0 :NewEnumerator16 2.0 :NewEnumerator17 1.0 :NewEnumerator18 1.0))
  (bind _returnvalue_6 (Utilities|Select :Index _breath_2 :NewEnumerator20 _returnvalue_4 :NewEnumerator0 "(R=0.392157,G=0.113725,B=0.007843,A=1.000000)" :NewEnumerator1 "(R=0.011765,G=0.023529,B=0.184314,A=1.000000)" :NewEnumerator2 "(R=0.949020,G=1.000000,B=0.000000,A=1.000000)" :NewEnumerator3 "(R=1.000000,G=0.474510,B=0.941177,A=1.000000)" :NewEnumerator4 "(R=0.301961,G=0.396078,B=0.396078,A=1.000000)" :NewEnumerator5 "(R=0.000000,G=0.301961,B=0.298039,A=1.000000)" :NewEnumerator6 "(R=0.075978,G=0.104167,B=0.003887,A=1.000000)" :NewEnumerator7 "(R=0.043137,G=1.000000,B=0.000000,A=1.000000)" :NewEnumerator8 "(R=0.302083,G=0.000000,B=0.017537,A=1.000000)" :NewEnumerator9 "(R=0.001703,G=0.000000,B=0.026042,A=1.000000)" :NewEnumerator10 "(R=0.963542,G=0.115260,B=0.000000,A=1.000000)" :NewEnumerator11 "(R=0.392157,G=0.113725,B=0.007843,A=1.000000)" :NewEnumerator12 "(R=0.011765,G=0.023529,B=0.184314,A=1.000000)" :NewEnumerator13 "(R=0.043137,G=1.000000,B=0.000000,A=1.000000)" :NewEnumerator14 "(R=0.583333,G=0.024500,B=0.027815,A=1.000000)" :NewEnumerator15 "(R=0.109804,G=1.000000,B=0.184314,A=1.000000)" :NewEnumerator16 "(R=1.000000,G=1.000000,B=1.000000,A=1.000000)" :NewEnumerator17 "(R=0.411765,G=0.000000,B=1.000000,A=1.000000)" :NewEnumerator18 "(R=0.011765,G=0.000000,B=0.070588,A=1.000000)"))
  (if (Variables|FairyAbilities|GetSuperfly)
    (Rendering|Material|SetMaterial _mesh 4 "/Game/SpyroContent/Global_Assets/Global_Materials/Material_Instances/Invisible_Mat.Invisible_Mat")
    (else
      (Rendering|Material|SetMaterial _mesh 3 "/Game/SpyroContent/Global_Assets/Global_Materials/Material_Instances/Invisible_Mat.Invisible_Mat")
      ;[1 1 1] wings
      (bind _returnvalue_7 (Rendering|Material|CreateDynamicMaterialInstance (Variables|Character|GetMesh) 4 "/Game/SpyroContent/Global_Assets/Global_Materials/Material_Instances/Untex_Vertex_Color_2Sided.Untex_Vertex_Color_2Sided" "None" :!class /Script/Engine.PrimitiveComponent))
      (Rendering|Material|SetVectorParameterValue _returnvalue_7 "ColorChange" (Utilities|Select :Index _breath :NewEnumerator20 "(R=0.521569,G=0.941177,B=1.000000,A=1.000000)" :NewEnumerator0 "(R=1.000000,G=0.721569,B=0.000000,A=1.000000)" :NewEnumerator1 "(R=0.243137,G=0.305882,B=1.000000,A=1.000000)" :NewEnumerator2 "(R=0.000000,G=1.000000,B=0.890196,A=1.000000)" :NewEnumerator3 "(R=0.498039,G=1.000000,B=1.000000,A=1.000000)" :NewEnumerator4 "(R=0.775102,G=1.000000,B=1.000000,A=1.000000)" :NewEnumerator5 "(R=0.188235,G=0.733333,B=0.729412,A=1.000000)" :NewEnumerator6 "(R=0.239331,G=0.328125,B=0.012245,A=1.000000)" :NewEnumerator7 "(R=0.043137,G=1.000000,B=0.000000,A=1.000000)" :NewEnumerator8 "(R=1.000000,G=0.000000,B=0.058054,A=1.000000)" :NewEnumerator9 "(R=0.008176,G=0.000000,B=0.125000,A=1.000000)" :NewEnumerator10 "(R=0.521569,G=0.941177,B=1.000000,A=1.000000)" :NewEnumerator11 "(R=1.000000,G=0.721569,B=0.000000,A=1.000000)" :NewEnumerator12 "(R=0.243137,G=0.305882,B=1.000000,A=1.000000)" :NewEnumerator13 "(R=0.043137,G=1.000000,B=0.000000,A=1.000000)" :NewEnumerator14 "(R=1.000000,G=0.721569,B=0.000000,A=1.000000)" :NewEnumerator15 "(R=0.109939,G=1.000000,B=0.183992,A=1.000000)" :NewEnumerator16 "(R=1.000000,G=1.000000,B=1.000000,A=1.000000)" :NewEnumerator17 "(R=0.203922,G=0.000000,B=1.000000,A=1.000000)" :NewEnumerator18 "(R=0.026552,G=0.000000,B=0.130208,A=1.000000)") :!class /Script/Engine.MaterialInstanceDynamic)
      (Rendering|Material|SetScalarParameterValue _returnvalue_7 "Brightness" (Utilities|Select :Index _breath :NewEnumerator20 1.0 :NewEnumerator0 2.0 :NewEnumerator1 1.0 :NewEnumerator2 1.0 :NewEnumerator3 2.0 :NewEnumerator4 1.0 :NewEnumerator5 1.0 :NewEnumerator6 1.0 :NewEnumerator7 1.0 :NewEnumerator8 1.0 :NewEnumerator9 1.0 :NewEnumerator10 1.0 :NewEnumerator11 2.0 :NewEnumerator12 1.0 :NewEnumerator13 1.0 :NewEnumerator14 2.0 :NewEnumerator15 1.0 :NewEnumerator16 1.0 :NewEnumerator17 1.0 :NewEnumerator18 1.0) :!class /Script/Engine.MaterialInstanceDynamic)
      (Rendering|Material|SetScalarParameterValue _returnvalue_7 "Opacity" 0.3 :!class /Script/Engine.MaterialInstanceDynamic)))
  (if (Variables|FairyAbilities|GetSupercharge)
    _
    (else
      (Rendering|Material|SetMaterial (Variables|Character|GetMesh) 12 "/Game/SpyroContent/Global_Assets/Global_Materials/Material_Instances/Invisible_Mat.Invisible_Mat")))
  (if (Variables|FairyAbilities|GetSuperinvincibility)
    (bind _asfairy_abp (Utilities|Casting|CastToFairy_ABP (Components|SkeletalMesh|GetAnimInstance (Variables|Character|GetMesh)))
      (:then
        (Variables|/Game/SpyroContent/Global_Assets/Global_Characters/NPCs/Fairies/Fairy_ABP.Fairy_ABP_C|SetABP_Invincibility _asfairy_abp true))
      (:CastFailed
        _))
    (else
      (Rendering|Material|SetMaterial (Variables|Character|GetMesh) 5 "/Game/SpyroContent/Global_Assets/Global_Materials/Material_Instances/Invisible_Mat.Invisible_Mat")))
  (if (Variables|FairyAbilities|GetInfinite)
    _
    (else
      (Rendering|Material|SetMaterial (Variables|Character|GetMesh) 2 "/Game/SpyroContent/Global_Assets/Global_Materials/Material_Instances/Invisible_Mat.Invisible_Mat")))
  ;[1 1 1] skin
  (bind _returnvalue_8 (Rendering|Material|CreateDynamicMaterialInstance (Variables|Character|GetMesh) 6 "/Game/SpyroContent/Global_Assets/Global_Materials/Material_Instances/Untex_Vertex_Color.Untex_Vertex_Color" "None" :!class /Script/Engine.PrimitiveComponent))
  (Rendering|Material|SetVectorParameterValue _returnvalue_8 "ColorChange" (Utilities|Select :Index (Variables|FairyAbilities|GetBreath) :NewEnumerator20 (select (or (Variables|FairyAbilities|GetSupercharge) (Variables|FairyAbilities|GetSuperinvincibility)) "(R=0.567708,G=0.257315,B=0.166104,A=1.000000)" "(R=1.000000,G=0.320595,B=0.160375,A=1.000000)") :NewEnumerator0 "(R=1.000000,G=0.262745,B=0.000000,A=1.000000)" :NewEnumerator1 "(R=0.062745,G=0.141176,B=1.000000,A=1.000000)" :NewEnumerator2 "(R=0.971058,G=1.000000,B=0.432292,A=1.000000)" :NewEnumerator3 "(R=0.744792,G=1.000000,B=1.000000,A=1.000000)" :NewEnumerator4 "(R=0.775102,G=1.000000,B=1.000000,A=1.000000)" :NewEnumerator5 "(R=0.188235,G=0.733333,B=0.729412,A=1.000000)" :NewEnumerator6 "(R=0.239331,G=0.328125,B=0.012245,A=1.000000)" :NewEnumerator7 "(R=0.250980,G=1.000000,B=0.215686,A=1.000000)" :NewEnumerator8 "(R=1.000000,G=0.000000,B=0.058054,A=1.000000)" :NewEnumerator9 "(R=0.008176,G=0.000000,B=0.125000,A=1.000000)" :NewEnumerator10 "(R=0.854000,G=0.238847,B=0.151229,A=1.000000)" :NewEnumerator11 "(R=1.000000,G=0.262745,B=0.000000,A=1.000000)" :NewEnumerator12 "(R=0.062745,G=0.141176,B=1.000000,A=1.000000)" :NewEnumerator13 "(R=0.250980,G=1.000000,B=0.215686,A=1.000000)" :NewEnumerator14 "(R=1.000000,G=0.262745,B=0.000000,A=1.000000)" :NewEnumerator15 "(R=0.443137,G=0.780392,B=0.470588,A=1.000000)" :NewEnumerator16 "(R=0.039216,G=0.039216,B=0.039216,A=1.000000)" :NewEnumerator17 "(R=0.534314,G=0.208333,B=1.000000,A=1.000000)" :NewEnumerator18 "(R=0.006944,G=0.000000,B=0.041667,A=1.000000)") :!class /Script/Engine.MaterialInstanceDynamic)
  ;[1 1 1] dress
  (bind _returnvalue_9 (CallFunction|IsFairySuper?))
  (bind _returnvalue_10 (Rendering|Material|CreateDynamicMaterialInstance (Variables|Character|GetMesh) 10 (select _returnvalue_9 "/Game/SpyroContent/Global_Assets/Global_Characters/NPCs/Fairies/Materials/Superfairy_Dress_Mat.Superfairy_Dress_Mat" "/Game/SpyroContent/Global_Assets/Global_Materials/Material_Instances/Untex_Vertex_Color.Untex_Vertex_Color") "None" :!class /Script/Engine.PrimitiveComponent))
  (Rendering|Material|SetVectorParameterValue _returnvalue_10 "ColorChange" (Utilities|Select :Index (Variables|FairyAbilities|GetBreath) :NewEnumerator20 (select (or (Variables|FairyAbilities|GetSupercharge) (Variables|FairyAbilities|GetSuperinvincibility)) "(R=0.218750,G=0.218750,B=0.218750,A=1.000000)" (select (Variables|FairyAbilities|GetSuperfly) "(R=0.196231,G=0.095732,B=0.526000,A=1.000000)" "(R=1.000000,G=0.000000,B=0.033201,A=1.000000)")) :NewEnumerator0 "(R=1.000000,G=0.149020,B=0.000000,A=1.000000)" :NewEnumerator1 "(R=0.011765,G=0.023529,B=0.184314,A=1.000000)" :NewEnumerator2 "(R=0.949020,G=1.000000,B=0.000000,A=1.000000)" :NewEnumerator3 "(R=1.000000,G=0.474510,B=0.941177,A=1.000000)" :NewEnumerator4 "(R=0.301961,G=0.396078,B=0.396078,A=1.000000)" :NewEnumerator5 "(R=0.000000,G=0.301961,B=0.298039,A=1.000000)" :NewEnumerator6 "(R=0.075978,G=0.104167,B=0.003887,A=1.000000)" :NewEnumerator7 "(R=0.043137,G=1.000000,B=0.000000,A=1.000000)" :NewEnumerator8 "(R=0.302083,G=0.000000,B=0.017537,A=1.000000)" :NewEnumerator9 "(R=0.001703,G=0.000000,B=0.026042,A=1.000000)" :NewEnumerator10 "(R=0.235294,G=0.015686,B=0.282353,A=1.000000)" :NewEnumerator11 "(R=1.000000,G=0.149020,B=0.000000,A=1.000000)" :NewEnumerator12 "(R=0.011765,G=0.023529,B=0.184314,A=1.000000)" :NewEnumerator13 "(R=0.043137,G=1.000000,B=0.000000,A=1.000000)" :NewEnumerator14 "(R=0.505208,G=0.000000,B=0.023774,A=1.000000)" :NewEnumerator15 "(R=0.109804,G=1.000000,B=0.184314,A=1.000000)" :NewEnumerator16 "(R=1.000000,G=1.000000,B=1.000000,A=1.000000)" :NewEnumerator17 "(R=0.411765,G=0.000000,B=1.000000,A=1.000000)" :NewEnumerator18 "(R=0.011765,G=0.000000,B=0.070588,A=1.000000)") :!class /Script/Engine.MaterialInstanceDynamic)
  (Rendering|Material|SetScalarParameterValue _returnvalue_10 "Brightness" (Utilities|Select :Index (Variables|FairyAbilities|GetBreath) :NewEnumerator20 2.0 :NewEnumerator0 2.0 :NewEnumerator1 2.0 :NewEnumerator2 2.0 :NewEnumerator3 6.0 :NewEnumerator4 6.0 :NewEnumerator5 2.0 :NewEnumerator6 1.0 :NewEnumerator7 1.0 :NewEnumerator8 1.0 :NewEnumerator9 1.0 :NewEnumerator10 1.0 :NewEnumerator11 2.0 :NewEnumerator12 1.0 :NewEnumerator13 1.0 :NewEnumerator14 2.0 :NewEnumerator15 2.0 :NewEnumerator16 2.0 :NewEnumerator17 1.0 :NewEnumerator18 1.0) :!class /Script/Engine.MaterialInstanceDynamic)
  (Rendering|Material|SetScalarParameterValue _returnvalue_10 "Flash Brightness" (Utilities|Select :Index (Variables|FairyAbilities|GetBreath) :NewEnumerator20 4.0 :NewEnumerator0 2.0 :NewEnumerator1 1e+01 :NewEnumerator2 2.0 :NewEnumerator3 2.0 :NewEnumerator4 2.0 :NewEnumerator5 2.0 :NewEnumerator6 2.0 :NewEnumerator7 2.0 :NewEnumerator8 2.0 :NewEnumerator9 2.0 :NewEnumerator10 4.0 :NewEnumerator11 2.0 :NewEnumerator12 1e+01 :NewEnumerator13 2.0 :NewEnumerator14 2.0 :NewEnumerator15 2.0 :NewEnumerator16 2.0 :NewEnumerator17 4.0 :NewEnumerator18 1e+01) :!class /Script/Engine.MaterialInstanceDynamic)
  ;[1 1 1] lips
  (bind _returnvalue_11 (Rendering|Material|CreateDynamicMaterialInstance (Variables|Character|GetMesh) 9 "/Game/SpyroContent/Global_Assets/Global_Materials/Material_Instances/Untex_Vertex_Color.Untex_Vertex_Color" "None" :!class /Script/Engine.PrimitiveComponent))
  (Rendering|Material|SetVectorParameterValue _returnvalue_11 "ColorChange" (Utilities|Select :Index (Variables|FairyAbilities|GetBreath) :NewEnumerator20 "(R=0.770833,G=0.020042,B=0.039768,A=1.000000)" :NewEnumerator0 "(R=1.000000,G=0.027451,B=0.000000,A=1.000000)" :NewEnumerator1 "(R=0.062745,G=0.141176,B=1.000000,A=1.000000)" :NewEnumerator2 "(R=0.949020,G=1.000000,B=0.000000,A=1.000000)" :NewEnumerator3 "(R=1.000000,G=0.474510,B=0.941177,A=1.000000)" :NewEnumerator4 "(R=0.206163,G=0.395833,B=0.395833,A=1.000000)" :NewEnumerator5 "(R=0.000000,G=0.224946,B=0.270833,A=1.000000)" :NewEnumerator6 "(R=0.075978,G=0.104167,B=0.003887,A=1.000000)" :NewEnumerator7 "(R=0.043137,G=1.000000,B=0.000000,A=1.000000)" :NewEnumerator8 "(R=0.302083,G=0.000000,B=0.017537,A=1.000000)" :NewEnumerator9 "(R=0.001703,G=0.000000,B=0.026042,A=1.000000)" :NewEnumerator10 "(R=0.630208,G=0.016412,B=0.029152,A=1.000000)" :NewEnumerator11 "(R=1.000000,G=0.027451,B=0.000000,A=1.000000)" :NewEnumerator12 "(R=0.062745,G=0.141176,B=1.000000,A=1.000000)" :NewEnumerator13 "(R=0.043137,G=1.000000,B=0.000000,A=1.000000)" :NewEnumerator14 "(R=1.000000,G=0.027451,B=0.000000,A=1.000000)" :NewEnumerator15 "(R=0.109804,G=1.000000,B=0.184314,A=1.000000)" :NewEnumerator16 "(R=0.039216,G=0.039216,B=0.039216,A=1.000000)" :NewEnumerator17 "(R=0.045670,G=0.000000,B=0.223958,A=1.000000)" :NewEnumerator18 "(R=0.000000,G=0.000000,B=0.000000,A=1.000000)") :!class /Script/Engine.MaterialInstanceDynamic)
  ;[1 1 1] eyes
  (bind _returnvalue_12 (Rendering|Material|CreateDynamicMaterialInstance (Variables|Character|GetMesh) 7 "/Game/SpyroContent/Global_Assets/Global_Characters/NPCs/Fairies/Materials/Fairy_Eyes_Mat.Fairy_Eyes_Mat" "None" :!class /Script/Engine.PrimitiveComponent))
  (Rendering|Material|SetVectorParameterValue _returnvalue_12 "ColorChange" (Utilities|Select :Index (Variables|FairyAbilities|GetBreath) :NewEnumerator20 "(R=0.009406,G=0.447917,B=0.025850,A=1.000000)" :NewEnumerator0 "(R=1.000000,G=0.027451,B=0.000000,A=1.000000)" :NewEnumerator1 "(R=0.000000,G=0.083677,B=1.000000,A=1.000000)" :NewEnumerator2 "(R=0.000000,G=1.000000,B=0.890196,A=1.000000)" :NewEnumerator3 "(R=1.000000,G=0.474510,B=0.941177,A=1.000000)" :NewEnumerator4 "(R=0.206163,G=0.395833,B=0.395833,A=1.000000)" :NewEnumerator5 "(R=0.000000,G=0.306000,B=1.000000,A=1.000000)" :NewEnumerator6 "(R=0.281118,G=0.385417,B=0.014382,A=1.000000)" :NewEnumerator7 "(R=0.043139,G=1.000000,B=0.000000,A=1.000000)" :NewEnumerator8 "(R=1.000000,G=0.000000,B=0.058053,A=1.000000)" :NewEnumerator9 "(R=0.001703,G=0.000000,B=0.026042,A=1.000000)" :NewEnumerator10 "(R=0.000000,G=0.588542,B=0.112055,A=1.000000)" :NewEnumerator11 "(R=1.000000,G=0.027451,B=0.000000,A=1.000000)" :NewEnumerator12 "(R=0.000000,G=0.082353,B=1.000000,A=1.000000)" :NewEnumerator13 "(R=0.043137,G=1.000000,B=0.000000,A=1.000000)" :NewEnumerator14 "(R=1.000000,G=0.027451,B=0.000000,A=1.000000)" :NewEnumerator15 "(R=0.109937,G=1.000000,B=0.183993,A=1.000000)" :NewEnumerator16 "(R=1.000000,G=1.000000,B=1.000000,A=1.000000)" :NewEnumerator17 "(R=0.299286,G=0.119792,B=1.000000,A=1.000000)" :NewEnumerator18 "(R=1.000000,G=0.000000,B=0.054682,A=1.000000)") :!class /Script/Engine.MaterialInstanceDynamic)
  ;[1 1 1] brows
  (bind _returnvalue_13 (Rendering|Material|CreateDynamicMaterialInstance (Variables|Character|GetMesh) 11 "/Game/SpyroContent/Global_Assets/Global_Characters/NPCs/Fairies/Materials/Fairy_Eyes_Mat.Fairy_Eyes_Mat" "None" :!class /Script/Engine.PrimitiveComponent))
  (Rendering|Material|SetVectorParameterValue _returnvalue_13 "ColorChange" _returnvalue_6 :!class /Script/Engine.MaterialInstanceDynamic)
  (Rendering|Material|SetScalarParameterValue _returnvalue_13 "Brightness" (* _returnvalue_5 2.0) :!class /Script/Engine.MaterialInstanceDynamic)
  ;[1 1 1] Hair
  (bind _returnvalue_14 (CallFunction|IsFairySuper?))
  (if _returnvalue_14
    (Rendering|Material|SetMaterial (Variables|Character|GetMesh) 1 "/Game/SpyroContent/Global_Assets/Global_Materials/Material_Instances/Invisible_Mat.Invisible_Mat")
    (bind _returnvalue_15 (Rendering|Material|CreateDynamicMaterialInstance (Variables|Character|GetMesh) 0 "/Game/SpyroContent/Global_Assets/Global_Materials/Material_Instances/Untex_Vertex_Color.Untex_Vertex_Color" "None" :!class /Script/Engine.PrimitiveComponent))
    (Rendering|Material|SetVectorParameterValue _returnvalue_15 "ColorChange" _returnvalue_6 :!class /Script/Engine.MaterialInstanceDynamic)
    (Rendering|Material|SetScalarParameterValue _returnvalue_15 "Brightness" _returnvalue_5 :!class /Script/Engine.MaterialInstanceDynamic)
    (else
      (Rendering|Material|SetMaterial (Variables|Character|GetMesh) 0 "/Game/SpyroContent/Global_Assets/Global_Materials/Material_Instances/Invisible_Mat.Invisible_Mat")
      (bind _returnvalue_16 (Rendering|Material|CreateDynamicMaterialInstance (Variables|Character|GetMesh) 1 "/Game/SpyroContent/Global_Assets/Global_Materials/Material_Instances/Untex_Vertex_Color.Untex_Vertex_Color" "None" :!class /Script/Engine.PrimitiveComponent))
      (Rendering|Material|SetVectorParameterValue _returnvalue_16 "ColorChange" _returnvalue_6 :!class /Script/Engine.MaterialInstanceDynamic)
      (Rendering|Material|SetScalarParameterValue _returnvalue_16 "Brightness" _returnvalue_5 :!class /Script/Engine.MaterialInstanceDynamic)))
  (bind _returnvalue_17 (Rendering|Material|CreateDynamicMaterialInstance (Variables|Character|GetMesh) 8 "/Game/SpyroContent/Global_Assets/Global_Materials/Material_Instances/Untex_Vertex_Color.Untex_Vertex_Color" "None" :!class /Script/Engine.PrimitiveComponent))
  (Rendering|Material|SetVectorParameterValue _returnvalue_17 "ColorChange" _returnvalue_6 :!class /Script/Engine.MaterialInstanceDynamic)
  (Rendering|Material|SetScalarParameterValue _returnvalue_17 "Brightness" _returnvalue_5 :!class /Script/Engine.MaterialInstanceDynamic)
  ;[1 1 1] dress overlap for super fairies
  (bind _returnvalue_18 (CallFunction|IsFairySuper?))
  (if _returnvalue_18
    _
    (else
      (Rendering|Material|SetMaterial (Variables|Character|GetMesh) 13 "/Game/SpyroContent/Global_Assets/Global_Materials/Material_Instances/Invisible_Mat.Invisible_Mat")))
  ;[1 1 1] Hearts
  (bind _returnvalue_19 (Rendering|Material|CreateDynamicMaterialInstance (Variables|Default|GetHeart_Particles) 0 "/Game/SpyroContent/Global_Assets/Global_Characters/NPCs/Fairies/Textures/hearts_mat.hearts_mat" "None" :!class /Script/Engine.PrimitiveComponent))
  (Rendering|Material|SetVectorParameterValue _returnvalue_19 "ColorChange" (Utilities|Select :Index (Variables|FairyAbilities|GetBreath) :NewEnumerator20 "(R=0.741176,G=0.109804,B=0.207843,A=1.000000)" :NewEnumerator0 "(R=0.964706,G=0.113725,B=0.000000,A=1.000000)" :NewEnumerator1 "(R=0.000000,G=0.058824,B=0.619608,A=1.000000)" :NewEnumerator2 "(R=0.949020,G=1.000000,B=0.000000,A=1.000000)" :NewEnumerator3 "(R=1.000000,G=0.474510,B=0.941177,A=1.000000)" :NewEnumerator4 "(R=0.301961,G=0.396078,B=0.396078,A=1.000000)" :NewEnumerator5 "(R=0.000000,G=1.000000,B=0.987012,A=1.000000)" :NewEnumerator6 "(R=0.186146,G=0.255208,B=0.009523,A=1.000000)" :NewEnumerator7 "(R=0.043137,G=1.000000,B=0.000000,A=1.000000)" :NewEnumerator8 "(R=1.000000,G=0.000000,B=0.058053,A=1.000000)" :NewEnumerator9 "(R=0.016349,G=0.000000,B=0.250000,A=1.000000)" :NewEnumerator10 "(R=1.000000,G=0.010000,B=0.414225,A=1.000000)" :NewEnumerator11 "(R=0.964706,G=0.113725,B=0.000000,A=1.000000)" :NewEnumerator12 "(R=0.000000,G=0.058824,B=0.619608,A=1.000000)" :NewEnumerator13 "(R=0.043137,G=1.000000,B=0.000000,A=1.000000)" :NewEnumerator14 "(R=0.964706,G=0.113725,B=0.000000,A=1.000000)" :NewEnumerator15 "(R=0.109804,G=1.000000,B=0.184314,A=1.000000)" :NewEnumerator16 "(R=1.000000,G=1.000000,B=1.000000,A=1.000000)" :NewEnumerator17 "(R=0.411765,G=0.000000,B=1.000000,A=1.000000)" :NewEnumerator18 "(R=0.036459,G=0.000000,B=0.218750,A=1.000000)") :!class /Script/Engine.MaterialInstanceDynamic))

(fn DoesFairyGiveSuperBreath?
  (bind _breath (Variables|FairyAbilities|GetBreath))
  (return (Math|Boolean|ORBoolean (Utilities|Enum|Equal(Enum) _breath "NewEnumerator10") (Utilities|Enum|Equal(Enum) _breath "NewEnumerator11") (Utilities|Enum|Equal(Enum) _breath "NewEnumerator12") (Utilities|Enum|Equal(Enum) _breath "NewEnumerator13") (Utilities|Enum|Equal(Enum) _breath "NewEnumerator14") (Utilities|Enum|Equal(Enum) _breath "NewEnumerator15") (Utilities|Enum|Equal(Enum) _breath "NewEnumerator16") (Utilities|Enum|Equal(Enum) _breath "NewEnumerator17") (Utilities|Enum|Equal(Enum) _breath "NewEnumerator18"))))

(fn CheckforPowerUpTargets
  (bind _kiss_radius (Variables|Default|GetKiss_Radius))
  (bind _kiss_radius_2 (Variables|Default|GetKiss_Radius))
  (bind _returnvalue (Transformation|GetWorldLocation _kiss_radius))
  (bind _outhits (Collision|MultiSphereTraceForObjects _returnvalue _returnvalue (* (Variables|/Script/Engine.SphereComponent|GetSphereRadius _kiss_radius_2) (.z (Variables|/Script/Engine.SceneComponent|GetRelativeScale3D _kiss_radius_2))) (Utilities|Array|MakeArray "ObjectTypeQuery3" "ObjectTypeQuery8" "ObjectTypeQuery9") false 0 "None" true "(R=0.838902,G=0.000000,B=1.000000,A=1.000000)" "(R=0.000000,G=1.000000,B=0.000000,A=1.000000)" 0.5))
  (for _array_element _outhits
    (if (.bblockinghit _array_element)
      (bind _asbp_base_playable (Utilities|Casting|CastToBP_Base_Playable (.hitactor _array_element)))
      (if (<= (Variables|/Game/SpyroContent/Global_Assets/Global_Characters/Playable_Characters/BP_Base_Playable.BP_Base_Playable_C|GetPowerUp_Time_Remaining _asbp_base_playable) 0.0)
        (CallFunction|Kiss (.hitactor _array_element) (.hitcomponent _array_element))))))