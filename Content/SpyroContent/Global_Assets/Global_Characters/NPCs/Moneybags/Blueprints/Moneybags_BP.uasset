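; Moneybags NPC, a dialogue character who charges the player a gem fee when a paying choice is submitted (first, optionally second).
; Payment is blocked if already paid, unaffordable, or during death, respawn, portal or homeworld transitions.
; A resettable DoOnce guards the charge, which commits collected gems and adds the cost to a saved gems-taken total.
; Success fires MoneybagsTookGems and switches to post-purchase dialogue; failure switches to can't-afford dialogue.
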(event Custom|Reset%20Take%20Player's%20Gems
  (Utilities|FlowControl|DoOnce false) ; enters at Reset
)

(event EventInvokedUISubmit
  (Utilities|FlowControl|Sequence
    (:then_0
      (Development|PrintString "Moneybags 0: ui submit occured")
      (if (== (Variables|Default|GetChosen_Choice_Number) 0)
        (bind _is_it_okay_1 (CallFunction|IsItOkaytoTakeGemsRightNow? :!label _label))
        (if _is_it_okay_1
          (Development|PrintString "Moneybags 1: do once")
          (Utilities|FlowControl|DoOnce false
            (:Completed
              (Development|PrintString "Moneybags 2: do once wasnt locked")
              (bind _asspyro_save_data (CallFunction|LoadSpyroGame self))
              (bind _player_who_last_spoke_to_moneybags (Variables|Default|GetPlayer%20Who%20Last%20Spoke%20to%20Moneybags)
                (:then
                  (bind _my_hud_ref (Variables|/Game/SpyroContent/Global_Assets/Global_Characters/Playable_Characters/Spyro_PlayerController.Spyro_PlayerController_C|GetMy_HUD_Ref _player_who_last_spoke_to_moneybags)
                    (:then
                      (if (>= (- (Variables|/Game/SpyroContent/Global_Assets/Global_UserInterface/Widgets/HUD.HUD_C|GetActual_HUD_Gems _my_hud_ref) (Variables|/Game/SpyroContent/Global_Assets/Global_SaveData/Spyro_SaveData.Spyro_SaveData_C|GetNumber_of_Gems_Moneybags_Took _asspyro_save_data)) (Variables|Default|GetMoneybags%20Gem%20Cost))
                        (Development|PrintString "CAN afford moneybags" true true "(R=0.000000,G=0.660000,B=1.000000,A=1.000000)" 3e+01)
                        (bind _asspyro_persistant_data (Utilities|Casting|CastToSpyro_PersistantData (Game|GetGameInstance))
                          (:then
                            (Default|CallPermanentlyCollectGems _asspyro_persistant_data)
                            (bind _foundwidgets (Widget|GetAllWidgetsOfClass "/Game/SpyroContent/Global_Assets/Global_UserInterface/Widgets/HUD.HUD_C" true))
                            (Default|SavePermanentGems (Utilities|Array|Get(acopy) _foundwidgets))
                            (bind (_asspyro_save_data_2 _as_persistent_data _slot_name) (CallFunction|LoadSpyroGame self))
                            (bind _player_who_last_spoke_to_moneybags_2 (Variables|Default|GetPlayer%20Who%20Last%20Spoke%20to%20Moneybags)
                              (:then
                                (bind _my_hud_ref_2 (Variables|/Game/SpyroContent/Global_Assets/Global_Characters/Playable_Characters/Spyro_PlayerController.Spyro_PlayerController_C|GetMy_HUD_Ref _player_who_last_spoke_to_moneybags_2)
                                  (:then
                                    (Variables|/Game/SpyroContent/Global_Assets/Global_UserInterface/Widgets/HUD.HUD_C|SetHUD_GemsMoneybagsTook _my_hud_ref_2 (+ (Variables|/Game/SpyroContent/Global_Assets/Global_SaveData/Spyro_SaveData.Spyro_SaveData_C|GetNumber_of_Gems_Moneybags_Took _asspyro_save_data_2) (Variables|Default|GetMoneybags%20Gem%20Cost)))
                                    (Variables|/Game/SpyroContent/Global_Assets/Global_SaveData/Spyro_SaveData.Spyro_SaveData_C|SetNumber_of_Gems_Moneybags_Took _asspyro_save_data_2 (+ (Variables|/Game/SpyroContent/Global_Assets/Global_SaveData/Spyro_SaveData.Spyro_SaveData_C|GetNumber_of_Gems_Moneybags_Took _asspyro_save_data_2) (Variables|Default|GetMoneybags%20Gem%20Cost)))
                                    (SaveGame|SaveGametoSlot _asspyro_save_data_2 _slot_name)
                                    (Variables|Default|SetMoneybags%20Was%20Paid true)
                                    (Default|CallMoneybagsTookGems)
                                    (Variables|Default|SetTalk_Again_Dialogue_Info (Variables|Default|GetPost-Purchase%20Dialogue))
                                    (bind _player_who_last_spoke_to_moneybags_3 (Variables|Default|GetPlayer%20Who%20Last%20Spoke%20to%20Moneybags)
                                      (:then
                                        (Default|ShowGemHUD _player_who_last_spoke_to_moneybags_3))
                                      (:else
                                        _))
                                    (CallFunction|ResetTakePlayer'sGems))
                                  (:else
                                    (CallFunction|ResetTakePlayer'sGems :!label _label_2)
                                    (Variables|Default|SetDialogue_Info (Variables|Default|GetCant%20Afford%20Me%20Dialogue) :!label _label_3)
                                    (Variables|Default|SetCant%20Afford%20Moneybags true)
                                    (Variables|Default|SetChosen_Choice_Number -1)
                                    (Variables|Default|SetCurrent_Dialogue_Index -1)
                                    (Development|PrintString "cant afford moneybags" true true "(R=0.000000,G=0.660000,B=1.000000,A=1.000000)" 3e+01))))
                              (:else
                                (goto _label_2))))
                          (:CastFailed
                            (goto _label_2)))
                        (else
                          (goto _label_2))))
                    (:else
                      (goto _label_2))))
                (:else
                  (goto _label_2)))))
          (else
            (Development|PrintString "Moneybags 1: it's not okay to take gems rn")
            (goto _label_3)))
        (else
          ;[0.207 0.03193 0.5573] qtderg experimental modification
          ;
          ; Second choice takes gems too - for holiday adventure
          (if (and (Variables|Default|GetSecond%20Choice%20Takes%20Gems%20Too) (== (Variables|Default|GetChosen_Choice_Number) 1))
            (goto _label)))))
    (:then_1
      (|CallParentFunction))))

(fn ConstructionScript
  (|CallParentFunction))

(fn IsAnyPlayerDying?
  (LocalVariables|SetA%20Player%20is%20Dying false)
  (bind _outactors (Actor|GetAllActorsOfClass "/Game/SpyroContent/Global_Assets/Global_Characters/Playable_Characters/BP_Base_Playable.BP_Base_Playable_C"))
  (bind _array_element (Utilities|Array|ForEachLoopwithBreak _outactors :!label _label)
    (:LoopBody
      (if (or (Utilities|Enum|Equal(Enum) (Variables|/Game/SpyroContent/Global_Assets/Global_Characters/Playable_Characters/BP_Base_Playable.BP_Base_Playable_C|GetPlayer_State _array_element) "NewEnumerator11") (Variables|/Game/SpyroContent/Global_Assets/Global_Characters/Playable_Characters/BP_Base_Playable.BP_Base_Playable_C|GetRespawning _array_element))
        (LocalVariables|SetA%20Player%20is%20Dying true)
        (goto _label Break)))
    (:Completed
      (return (LocalVariables|GetA%20Player%20is%20Dying)))))

(fn IsItOkaytoTakeGemsRightNow?
  (LocalVariables|SetIs%20it%20Okay? false)
  (Utilities|FlowControl|Sequence
    (:then_0
      (bind _a_players_dying (CallFunction|IsAnyPlayerDying?))
      (bind _asspyro_persistant_data (Utilities|Casting|CastToSpyro_PersistantData (Game|GetGameInstance)))
      (Variables|/Game/SpyroContent/Global_Assets/Global_SaveData/Spyro_PersistantData.Spyro_PersistantData_C|GetPlayer_in_Portal _asspyro_persistant_data
        (:then)
        (:else
          (if (Math|Boolean|ANDBoolean (not (Variables|Default|GetMoneybags%20Was%20Paid)) (not _a_players_dying) (not (Variables|/Game/SpyroContent/Global_Assets/Global_SaveData/Spyro_PersistantData.Spyro_PersistantData_C|GetSpecial_Homeworld_Transition _asspyro_persistant_data)) (not (Variables|Default|GetCant%20Afford%20Moneybags)))
            (LocalVariables|SetIs%20it%20Okay? true)))))
    (:then_1
      (return (LocalVariables|GetIs%20it%20Okay?)))))

(fn OnNPCTalkingStart
  (params (Player%20I%20Am%20Talking%20To :type BP%20Base%20Playable%20Object%20Reference))
  (|CallParentFunction Player%20I%20Am%20Talking%20To)
  (Variables|Default|SetCant%20Afford%20Moneybags false)
  (bind _talking_to (Variables|Default|GetTalking_To)
    (:then
      (bind _spyrocontr_ref (Variables|/Game/SpyroContent/Global_Assets/Global_Characters/Playable_Characters/BP_Base_Playable.BP_Base_Playable_C|GetSpyroContr_Ref _talking_to)
        (:then
          (Variables|Default|SetPlayer%20Who%20Last%20Spoke%20to%20Moneybags _spyrocontr_ref))
        (:else)))
    (:else)))

(fn OnNPCTalkingEnd
  (params (Player%20I%20Am%20Talking%20To :type BP%20Base%20Playable%20Object%20Reference))
  (|CallParentFunction Player%20I%20Am%20Talking%20To))