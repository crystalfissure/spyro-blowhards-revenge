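; Base character Blueprint for walking AI characters, handling player alert, death and respawn through its WalkingAICharacter, Damageable and DropsItems components.
; Radius overlaps and a looping sphere-trace ping alert it, optionally only when on camera, and raise its walk speed.
; Charging players damage it, and its launched corpse damages other Damageables before poofing on landing.
; DropsItems resets respawn it, with Hard and Nightmare difficulty, including Dynamic skill level, allowing respawns without remaining drops.
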(event OnComponentHit(CapsuleComponent)
  (params (HitComponent :type Primitive%20Component%20Object%20Reference) (OtherActor :type Actor%20Object%20Reference) (OtherComp :type Primitive%20Component%20Object%20Reference) (NormalImpulse :type Vector :default "0, 0, 0") (Hit :type Hit%20Result%20Structure%20%28by%20ref%29))
  (CallFunction|DoesMyCorpseDamageThisTarget? OtherActor OtherComp NormalImpulse))

(event OnComponentBeginOverlap(Alert_Radius)
  (params (OverlappedComponent :type Primitive%20Component%20Object%20Reference) (OtherActor :type Actor%20Object%20Reference) (OtherComp :type Primitive%20Component%20Object%20Reference) (OtherBodyIndex :type Integer) (bFromSweep :type Boolean) (SweepResult :type Hit%20Result%20Structure%20%28by%20ref%29))
  (CallFunction|ShouldThisPlayerMakeMeAlert? OtherActor OtherComp))

(event OnComponentBeginOverlap(CapsuleComponent)
  (params (OverlappedComponent :type Primitive%20Component%20Object%20Reference) (OtherActor :type Actor%20Object%20Reference) (OtherComp :type Primitive%20Component%20Object%20Reference) (OtherBodyIndex :type Integer) (bFromSweep :type Boolean) (SweepResult :type Hit%20Result%20Structure%20%28by%20ref%29))
  (bind _damageable (Variables|Default|GetDamageable))
  (bind _deal_damage___person_who_dealt_the_damage (Variables|/Game/SpyroContent/Global_Assets/Global_Components/Damageable_Com.Damageable_Com_C|GetDeal%20Damage%20-%20Person%20Who%20Dealt%20the%20Damage (Variables|Default|GetDamageable))
    (:then
      (CallFunction|DoesMyCorpseDamageThisTarget? OtherActor OtherComp (Transformation|GetActorForwardVector _deal_damage___person_who_dealt_the_damage)))
    (:else
      (CallFunction|DoesMyCorpseDamageThisTarget? OtherActor OtherComp "0, 0, 0")))
  (bind _asbp_base_playable (Utilities|Casting|CastToBP_Base_Playable OtherActor))
  (if (Math|Boolean|ANDBoolean (== (Variables|/Script/Engine.Character|GetCapsuleComponent _asbp_base_playable) OtherComp) (not (Utilities|Enum|Equal(Enum) (Variables|/Game/SpyroContent/Global_Assets/Global_Components/Base_AI_Character.Base_AI_Character_C|GetAICharacter_State (Variables|Default|GetWalking_AI_Character)) "NewEnumerator3")) (Utilities|Enum|Equal(Enum) (Variables|/Game/SpyroContent/Global_Assets/Global_Characters/Playable_Characters/BP_Base_Playable.BP_Base_Playable_C|GetPlayer_State _asbp_base_playable) "NewEnumerator4"))
    (bind _asbp_spyro (Utilities|Casting|CastToBP_Spyro _asbp_base_playable)
      (:then
        (Default|DealDamage _damageable "NewEnumerator4" (Transformation|GetActorForwardVector _asbp_base_playable) (Variables|/Game/SpyroContent/Global_Assets/Global_Characters/Playable_Characters/Spyro/BP_Spyro.BP_Spyro_C|Getis_Currently_Supercharging _asbp_spyro) _asbp_base_playable true))
      (:CastFailed
        (Default|DealDamage _damageable "NewEnumerator4" (Transformation|GetActorForwardVector _asbp_base_playable) false _asbp_base_playable true)))))

(event OnComponentEndOverlap(Unalert_Radius)
  (params (OverlappedComponent :type Primitive%20Component%20Object%20Reference) (OtherActor :type Actor%20Object%20Reference) (OtherComp :type Primitive%20Component%20Object%20Reference) (OtherBodyIndex :type Integer))
  (bind _walking_ai_character (Variables|Default|GetWalking_AI_Character))
  (bind _walking_ai_character_2 (Variables|Default|GetWalking_AI_Character))
  (bind _aicharacter_state (Variables|/Game/SpyroContent/Global_Assets/Global_Components/Base_AI_Character.Base_AI_Character_C|GetAICharacter_State _walking_ai_character))
  (bind _asbp_base_playable (Utilities|Casting|CastToBP_Base_Playable OtherActor))
  (if (and (== (Variables|/Script/Engine.Character|GetCapsuleComponent _asbp_base_playable) OtherComp) (or (Variables|/Game/SpyroContent/Global_Assets/Global_Components/Base_AI_Character.Base_AI_Character_C|GetCan_Become_Alert _walking_ai_character_2) (Variables|/Game/SpyroContent/Global_Assets/Global_Components/Base_AI_Character.Base_AI_Character_C|GetCan_Attack _walking_ai_character_2)))
    (Utilities|Array|RemoveItem (Variables|/Game/SpyroContent/Global_Assets/Global_Components/Base_AI_Character.Base_AI_Character_C|GetPlayers_I_Am_Alert_To (Variables|Default|GetWalking_AI_Character)) _asbp_base_playable)
    (if (Math|Boolean|ANDBoolean (== (Variables|/Script/Engine.Character|GetCapsuleComponent _asbp_base_playable) OtherComp) (or (and (Variables|/Game/SpyroContent/Global_Assets/Global_Components/Base_AI_Character.Base_AI_Character_C|GetCan_Become_Alert _walking_ai_character) (Utilities|Enum|Equal(Enum) _aicharacter_state "NewEnumerator1")) (and (Variables|/Game/SpyroContent/Global_Assets/Global_Components/Base_AI_Character.Base_AI_Character_C|GetCan_Attack _walking_ai_character) (Utilities|Enum|Equal(Enum) _aicharacter_state "NewEnumerator2"))) (<= (Utilities|Array|Length (Variables|/Game/SpyroContent/Global_Assets/Global_Components/Base_AI_Character.Base_AI_Character_C|GetPlayers_I_Am_Alert_To (Variables|Default|GetWalking_AI_Character))) 0))
      (Default|ChangeAICharacterState (Variables|Default|GetWalking_AI_Character) "NewEnumerator0")
      (Variables|/Script/Engine.CharacterMovementComponent|SetMaxWalkSpeed (Variables|Character|GetCharacterMovement) (Variables|Default|GetDefault%20Walk%20Speed)))))

(event Custom|Reset%20This%20AICharacter
  (bind _capsulecomponent (Variables|Collision|GetCapsuleComponent))
  (if (Variables|/Game/SpyroContent/Global_Assets/Global_Components/Drops_Items.Drops_Items_C|GetReset%20Even%20When%20Empty (Variables|Default|GetDrops_Items))
    (Transformation|SetActorLocation (Variables|/Game/SpyroContent/Global_Assets/Global_Components/Base_AI_Character.Base_AI_Character_C|GetSpawn_Point (Variables|Default|GetWalking_AI_Character)) false false :!label _label)
    (Default|ChangeAICharacterState (Variables|Default|GetWalking_AI_Character) "NewEnumerator0")
    (Rendering|SetActorHiddenInGame false)
    (Collision|SetCollisionResponsetoChannel _capsulecomponent "ECC_Pawn" "ECR_Block")
    (Collision|SetCollisionResponsetoChannel _capsulecomponent "ECC_GameTraceChannel2" "ECR_Block")
    (Collision|SetCollisionResponsetoChannel _capsulecomponent "ECC_GameTraceChannel4" "ECR_Overlap")
    (Collision|SetCollisionResponsetoChannel _capsulecomponent "ECC_Camera" "ECR_Block")
    (Collision|SetCollisionObjectType _capsulecomponent "ECC_Pawn")
    (bind _asbox_collision (Utilities|Casting|CastToBoxComponent (Variables|/Game/SpyroContent/Global_Assets/Global_Components/Damageable_Com.Damageable_Com_C|GetObject's%20Hitbox%20Component (Variables|Default|GetDamageable))))
    (Collision|SetCollisionResponsetoAllChannels _asbox_collision "ECR_Overlap")
    (Collision|SetCollisionObjectType _asbox_collision "ECC_Pawn")
    (else
      (bind _i_can_drop_items (Default|ShouldIDropAnyItems? (Variables|Default|GetDrops_Items)))
      (if _i_can_drop_items
        (goto _label)))))

(event Custom|On%20State%20Changed
  (if (Utilities|Enum|Equal(Enum) (Variables|/Game/SpyroContent/Global_Assets/Global_Components/Base_AI_Character.Base_AI_Character_C|GetAICharacter_State (Variables|Default|GetWalking_AI_Character)) "NewEnumerator3")
    (Audio|Components|Audio|Stop (Variables|Default|GetCharacter's%20Voice))
    (Utilities|FlowControl|Delay 0.5)
    (|corpsecollissionconditions)
    (Collision|SetCollisionObjectType (Variables|Collision|GetCapsuleComponent) "ECC_PhysicsBody")))

(event Custom|On%20Fairy%20Kiss
  (if (Utilities|Enum|Equal(Enum) (Variables|/Game/SpyroContent/Global_Assets/Global_Components/Base_AI_Character.Base_AI_Character_C|GetAICharacter_State (Variables|Default|GetWalking_AI_Character)) "NewEnumerator3")
    (bind _asspyro_universal_save_data (CallFunction|LoadUniversalSave))
    (if (Utilities|Enum|Equal(Enum) (Variables|/Game/SpyroContent/Global_Assets/Global_SaveData/Spyro_Universal_Save_Data.Spyro_Universal_Save_Data_C|GetDifficulty _asspyro_universal_save_data) "NewEnumerator4")
      (bind _asspyro_save_data (CallFunction|LoadSpyroGame self))
      (bind _difficulty (CallFunction|ConvertSkillLevelFloattoEnum (Variables|/Game/SpyroContent/Global_Assets/Global_SaveData/Spyro_SaveData.Spyro_SaveData_C|GetSkill_Level _asspyro_save_data)))
      (Variables|/Game/SpyroContent/Global_Assets/Global_Components/Drops_Items.Drops_Items_C|SetReset%20Even%20When%20Empty (Variables|Default|GetDrops_Items) (Utilities|Select :Index _difficulty :NewEnumerator4 false :NewEnumerator0 false :NewEnumerator1 false :NewEnumerator2 true :NewEnumerator3 true))
      (else
        (Variables|/Game/SpyroContent/Global_Assets/Global_Components/Drops_Items.Drops_Items_C|SetReset%20Even%20When%20Empty (Variables|Default|GetDrops_Items) (Utilities|Select :Index (Variables|/Game/SpyroContent/Global_Assets/Global_SaveData/Spyro_Universal_Save_Data.Spyro_Universal_Save_Data_C|GetDifficulty _asspyro_universal_save_data) :NewEnumerator4 false :NewEnumerator0 false :NewEnumerator1 false :NewEnumerator2 true :NewEnumerator3 true))))))

(event Custom|Disable%20Camera%20Col%20During%20Death%20Launch
  (bind _capsulecomponent (Variables|Collision|GetCapsuleComponent))
  (Collision|SetCollisionResponsetoChannel _capsulecomponent "ECC_Camera" "ECR_Ignore")
  (Collision|SetCollisionResponsetoChannel _capsulecomponent "ECC_Pawn" "ECR_Overlap"))

(event Custom|On%20Difficulty%20Changed
  (if (not (Variables|/Game/SpyroContent/Global_Assets/Global_Components/Drops_Items.Drops_Items_C|GetReset%20Even%20When%20Empty (Variables|Default|GetDrops_Items)))
    (bind _asspyro_universal_save_data (CallFunction|LoadUniversalSave))
    (switch Utilities|FlowControl|Switch|SwitchonDifficulty_Settings (Variables|/Game/SpyroContent/Global_Assets/Global_SaveData/Spyro_Universal_Save_Data.Spyro_Universal_Save_Data_C|GetDifficulty _asspyro_universal_save_data)
      (:NewEnumerator4
        (bind _asspyro_save_data (CallFunction|LoadSpyroGame self))
        (bind _difficulty (CallFunction|ConvertSkillLevelFloattoEnum (Variables|/Game/SpyroContent/Global_Assets/Global_SaveData/Spyro_SaveData.Spyro_SaveData_C|GetSkill_Level _asspyro_save_data)))
        (switch Utilities|FlowControl|Switch|SwitchonDifficulty_Settings _difficulty
          (:NewEnumerator2
            _)
          (:NewEnumerator3
            _)))
      (:NewEnumerator2
        _)
      (:NewEnumerator3
        _))
    (Variables|/Game/SpyroContent/Global_Assets/Global_Components/Drops_Items.Drops_Items_C|SetReset%20Even%20When%20Empty (Variables|Default|GetDrops_Items) true)))

(event EventBeginPlay
  (Variables|/Game/SpyroContent/Global_Assets/Global_Components/Damageable_Com.Damageable_Com_C|SetObject's%20Hitbox%20Component (Variables|Default|GetDamageable) (Variables|Collision|GetCapsuleComponent))
  (EventDispatchers|BindEventtoItemDropperSuccessfullyReset (Variables|Default|GetDrops_Items) (delegate Custom|Reset%20This%20AICharacter))
  (Utilities|Time|SetTimerbyFunctionName 0 "Alert Radius Ping" 0.5 true)
  (bind _asdropshadow_bp (Utilities|Casting|CastToDropshadow_BP (Variables|/Script/Engine.ChildActorComponent|GetChildActor (Variables|Default|GetAIs_DropShadow)))
    (:then
      (Variables|/Game/SpyroContent/Global_Assets/Global_Level_Items/Dropshadow/Dropshadow_BP.Dropshadow_BP_C|SetOwning%20Component _asdropshadow_bp (Variables|Character|GetMesh))
      (EventDispatchers|BindEventtoMyStateChanged (Variables|Default|GetWalking_AI_Character) (delegate Custom|On%20State%20Changed)))
    (:CastFailed
      _))
  (EventDispatchers|BindEventtoIWasKilledandLaunched (Variables|Default|GetWalking_AI_Character) (delegate Custom|Disable%20Camera%20Col%20During%20Death%20Launch))
  (bind _asspyro_persistant_data (Utilities|Casting|CastToSpyro_PersistantData (Game|GetGameInstance)))
  (EventDispatchers|BindEventtoAFairyKissedAPlayer _asspyro_persistant_data (delegate Custom|On%20Fairy%20Kiss))
  (EventDispatchers|BindEventtoDifficultyChanged _asspyro_persistant_data (delegate Custom|On%20Difficulty%20Changed)))

(event EventOnMovementModeChanged
  (params (PrevMovementMode :type EMovementMode%20Enum :default "MOVE_None") (NewMovementMode :type EMovementMode%20Enum :default "MOVE_None") (PrevCustomMode :type Byte :default 0) (NewCustomMode :type Byte :default 0))
  (if (Math|Boolean|ANDBoolean (Utilities|Enum|Equal(Enum) PrevMovementMode "MOVE_Falling") (Utilities|Enum|Equal(Enum) NewMovementMode "MOVE_Walking") (Utilities|Enum|Equal(Enum) (Variables|/Game/SpyroContent/Global_Assets/Global_Components/Base_AI_Character.Base_AI_Character_C|GetAICharacter_State (Variables|Default|GetWalking_AI_Character)) "NewEnumerator3") (not (Variables|Rendering|GetbHidden)) (not (Variables|/Game/SpyroContent/Global_Assets/Global_Components/Base_AI_Character.Base_AI_Character_C|GetPoofs_On_Death (Variables|Default|GetWalking_AI_Character))))
    (Default|DisableCollissionDuetoDeath (Variables|Default|GetWalking_AI_Character))
    (Utilities|FlowControl|Delay (Variables|Default|GetCorpse%20Poof%20Delay))
    (Default|PoofAwayCorpse (Variables|Default|GetWalking_AI_Character))))

(fn ConstructionScript
  (Variables|Default|SetDefault%20Walk%20Speed (Variables|/Script/Engine.CharacterMovementComponent|GetMaxWalkSpeed (Variables|Character|GetCharacterMovement))))

(fn DoesMyCorpseDamageThisTarget?
  (params (other%20actor :type Actor%20Object%20Reference) (other%20comp :type Object%20Object%20Reference) (Attacker's%20Forward%20Vector :type Vector))
  (bind _returnvalue (Actor|GetComponentbyClass other%20actor "/Game/SpyroContent/Global_Assets/Global_Components/Damageable_Com.Damageable_Com_C"))
  (Utilities|IsValid other%20actor
    (:Is%20Valid
      (Utilities|IsValid _returnvalue
        (:Is%20Valid
          (if (Math|Boolean|ANDBoolean (== (Variables|/Game/SpyroContent/Global_Assets/Global_Components/Damageable_Com.Damageable_Com_C|GetObject's%20Hitbox%20Component _returnvalue) other%20comp) (not (== other%20actor (Variables|/Game/SpyroContent/Global_Assets/Global_Components/Damageable_Com.Damageable_Com_C|GetDeal%20Damage%20-%20Person%20Who%20Dealt%20the%20Damage (Variables|Default|GetDamageable)))) (and (Utilities|Enum|Equal(Enum) (Variables|/Game/SpyroContent/Global_Assets/Global_Components/Base_AI_Character.Base_AI_Character_C|GetAICharacter_State (Variables|Default|GetWalking_AI_Character)) "NewEnumerator3") (AI|Components|NavMovement|IsFalling (Variables|Character|GetCharacterMovement))) (not (Variables|/Game/SpyroContent/Global_Assets/Global_Components/Base_AI_Character.Base_AI_Character_C|GetPoofs_On_Death (Variables|Default|GetWalking_AI_Character))))
            (Default|DealDamage _returnvalue "NewEnumerator4" Attacker's%20Forward%20Vector false (Variables|/Game/SpyroContent/Global_Assets/Global_Components/Damageable_Com.Damageable_Com_C|GetDeal%20Damage%20-%20Person%20Who%20Dealt%20the%20Damage (Variables|Default|GetDamageable)) false)))))))

(fn CheckifASpecificPlayerIsonCamera
  (params (player%20contr%20ref :type Player%20Controller%20Object%20Reference))
  (bind _returnvalue (Transformation|GetActorLocation))
  (bind _returnvalue_2 (Transformation|GetActorLocation))
  (bind _returnvalue_3 (Transformation|GetActorLocation))
  (bind _returnvalue_4 (Transformation|GetActorRightVector))
  (bind _returnvalue_5 (Transformation|GetActorLocation))
  (bind _returnvalue_6 (Transformation|GetActorLocation))
  (bind _returnvalue_7 (Transformation|GetActorRightVector))
  (bind _returnvalue_8 (Transformation|GetActorLocation))
  (bind _returnvalue_9 (Transformation|GetActorLocation))
  (bind _returnvalue_10 (Transformation|GetActorForwardVector))
  (bind _returnvalue_11 (Transformation|GetActorForwardVector))
  (bind _returnvalue_12 (Transformation|GetActorUpVector))
  (bind _returnvalue_13 (Transformation|GetActorUpVector))
  (bind _capsulecomponent (Variables|Collision|GetCapsuleComponent))
  (bind _capsulecomponent_2 (Variables|Collision|GetCapsuleComponent))
  (bind _capsulecomponent_3 (Variables|Collision|GetCapsuleComponent))
  (bind _capsulecomponent_4 (Variables|Collision|GetCapsuleComponent))
  (bind _capsulecomponent_5 (Variables|Collision|GetCapsuleComponent))
  (bind _capsulecomponent_6 (Variables|Collision|GetCapsuleComponent))
  (bind _screenlocation (Class|PlayerController|ProjectWorldLocationtoScreen player%20contr%20ref _returnvalue true))
  (bind _capsuleradius (Variables|/Script/Engine.CapsuleComponent|GetCapsuleRadius _capsulecomponent_2))
  (bind _capsulehalfheight (Variables|/Script/Engine.CapsuleComponent|GetCapsuleHalfHeight _capsulecomponent_3))
  (bind _capsulehalfheight_2 (Variables|/Script/Engine.CapsuleComponent|GetCapsuleHalfHeight _capsulecomponent))
  (bind _capsuleradius_2 (Variables|/Script/Engine.CapsuleComponent|GetCapsuleRadius _capsulecomponent_4))
  (bind _capsuleradius_3 (Variables|/Script/Engine.CapsuleComponent|GetCapsuleRadius _capsulecomponent_5))
  (bind _capsuleradius_4 (Variables|/Script/Engine.CapsuleComponent|GetCapsuleRadius _capsulecomponent_6))
  (bind _returnvalue_14 (* _returnvalue_13 _capsulehalfheight_2))
  (bind _returnvalue_15 (* _returnvalue_7 _capsuleradius_3))
  (bind _returnvalue_16 (* _returnvalue_11 _capsuleradius))
  (bind _returnvalue_17 (* _capsuleradius_2 -1.0))
  (bind _returnvalue_18 (* _capsuleradius_4 -1.0))
  (bind _returnvalue_19 (* _capsulehalfheight -1.0))
  (bind _returnvalue_20 (* _returnvalue_12 _returnvalue_19))
  (bind _returnvalue_21 (* _returnvalue_4 _returnvalue_17))
  (bind _returnvalue_22 (* _returnvalue_10 _returnvalue_18))
  (bind _returnvalue_23 (+ _returnvalue_5 _returnvalue_15))
  (bind _returnvalue_24 (+ _returnvalue_9 _returnvalue_16))
  (bind _returnvalue_25 (+ _returnvalue_6 _returnvalue_14))
  (bind _screenlocation_2 (Class|PlayerController|ProjectWorldLocationtoScreen player%20contr%20ref _returnvalue_25 true))
  (bind _screenlocation_3 (Class|PlayerController|ProjectWorldLocationtoScreen player%20contr%20ref _returnvalue_23 true))
  (bind _screenlocation_4 (Class|PlayerController|ProjectWorldLocationtoScreen player%20contr%20ref _returnvalue_24 true))
  (bind _returnvalue_26 (+ _returnvalue_2 _returnvalue_20))
  (bind _returnvalue_27 (+ _returnvalue_3 _returnvalue_21))
  (bind _returnvalue_28 (+ _returnvalue_8 _returnvalue_22))
  (bind _screenlocation_5 (Class|PlayerController|ProjectWorldLocationtoScreen player%20contr%20ref _returnvalue_26 true))
  (bind _screenlocation_6 (Class|PlayerController|ProjectWorldLocationtoScreen player%20contr%20ref _returnvalue_27 true))
  (bind _screenlocation_7 (Class|PlayerController|ProjectWorldLocationtoScreen player%20contr%20ref _returnvalue_28 true))
  (return (Math|Boolean|ORBoolean (and (> (.x _screenlocation) 0.0) (< (.x _screenlocation) (.x (Viewport|GetViewportSize)))) (and (> (.x _screenlocation_6) 0.0) (< (.x _screenlocation_6) (.x (Viewport|GetViewportSize)))) (and (> (.x _screenlocation_3) 0.0) (< (.x _screenlocation_3) (.x (Viewport|GetViewportSize)))) (and (> (.x _screenlocation_7) 0.0) (< (.x _screenlocation_7) (.x (Viewport|GetViewportSize)))) (and (> (.x _screenlocation_4) 0.0) (< (.x _screenlocation_4) (.x (Viewport|GetViewportSize)))) (and (> (.x _screenlocation_5) 0.0) (< (.x _screenlocation_5) (.x (Viewport|GetViewportSize)))) (and (> (.x _screenlocation_2) 0.0) (< (.x _screenlocation_2) (.x (Viewport|GetViewportSize)))))))

(fn AmIonCamera?
  (bind _walking_ai_character (Variables|Default|GetWalking_AI_Character))
  (bind _players_i_am_alert_to (Variables|/Game/SpyroContent/Global_Assets/Global_Components/Base_AI_Character.Base_AI_Character_C|GetPlayers_I_Am_Alert_To _walking_ai_character))
  (Utilities|FlowControl|Sequence
    (:then_0
      (LocalVariables|Setim%20on%20camera false)
      (if (Utilities|Array|IsValidIndex _players_i_am_alert_to)
        (bind _array_element (Utilities|Array|ForEachLoopwithBreak _players_i_am_alert_to :!label _label)
          (:LoopBody
            (bind _spyrocontr_ref (Variables|/Game/SpyroContent/Global_Assets/Global_Characters/Playable_Characters/BP_Base_Playable.BP_Base_Playable_C|GetSpyroContr_Ref _array_element)
              (:then
                (bind _returnvalue (CallFunction|CheckifASpecificPlayerIsonCamera _spyrocontr_ref))
                (LocalVariables|Setim%20on%20camera _returnvalue)
                (goto _label Break))
              (:else))))
        (else
          (bind _returnvalue_2 (CallFunction|CheckifASpecificPlayerIsonCamera (Game|GetPlayerController 0)))
          (LocalVariables|Setim%20on%20camera _returnvalue_2))))
    (:then_1
      (return (LocalVariables|Getim%20on%20camera)))))

(fn AlertRadiusPing
  (bind _alert_radius (Variables|Default|GetAlert_Radius))
  (bind _returnvalue (Transformation|GetWorldLocation _alert_radius))
  (bind _outhits (Collision|MultiSphereTraceForObjects _returnvalue _returnvalue (Variables|/Script/Engine.SphereComponent|GetSphereRadius _alert_radius) (Utilities|Array|MakeArray "ObjectTypeQuery3" "ObjectTypeQuery9" "ObjectTypeQuery8" "ObjectTypeQuery10") false 0 "None"))
  (for _array_element _outhits
    (bind _asbp_base_playable (Utilities|Casting|CastToBP_Base_Playable (.hitactor _array_element)))
    (CallFunction|ShouldThisPlayerMakeMeAlert? _asbp_base_playable (.hitcomponent _array_element))))

(fn ShouldThisPlayerMakeMeAlert?
  (params (Other%20Actor :type Object%20Object%20Reference) (Other%20Comp :type Object%20Object%20Reference))
  (bind _walking_ai_character (Variables|Default|GetWalking_AI_Character))
  (bind _walking_ai_character_2 (Variables|Default|GetWalking_AI_Character))
  (bind _asbp_base_playable (Utilities|Casting|CastToBP_Base_Playable Other%20Actor))
  (if (and (== (Variables|/Script/Engine.Character|GetCapsuleComponent _asbp_base_playable) Other%20Comp) (Variables|/Game/SpyroContent/Global_Assets/Global_Components/Base_AI_Character.Base_AI_Character_C|GetCan_Become_Alert _walking_ai_character_2))
    (if (Variables|/Game/SpyroContent/Global_Assets/Global_Components/Base_AI_Character.Base_AI_Character_C|GetCan't%20Be%20Alerted%20from%20Off%20Camera (Variables|Default|GetWalking_AI_Character))
      (bind _returnvalue (CallFunction|AmIonCamera?))
      (if _returnvalue
        (Utilities|Array|AddUnique (Variables|/Game/SpyroContent/Global_Assets/Global_Components/Base_AI_Character.Base_AI_Character_C|GetPlayers_I_Am_Alert_To _walking_ai_character) _asbp_base_playable :!label _label)
        (if (Utilities|Enum|Equal(Enum) (Variables|/Game/SpyroContent/Global_Assets/Global_Components/Base_AI_Character.Base_AI_Character_C|GetAICharacter_State _walking_ai_character_2) "NewEnumerator0")
          (Default|ChangeAICharacterState _walking_ai_character "NewEnumerator1")
          (Variables|/Script/Engine.CharacterMovementComponent|SetMaxWalkSpeed (Variables|Character|GetCharacterMovement) (* (Variables|Default|GetDefault%20Walk%20Speed) (Variables|Default|GetRun%20Speed%20Multiplier)))))
      (else
        (goto _label)))))