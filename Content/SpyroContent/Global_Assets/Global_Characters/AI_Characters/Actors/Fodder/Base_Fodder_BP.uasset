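; Base Blueprint for fodder AI characters that adds a chance of "lucky butterflies" when the fodder dies.
; On entering the Dying state, it reads the universal save's difficulty, with one setting deferring to the saved skill level.
; Two difficulty tiers get a weighted random roll to spawn a pair of butterflies beside it.
; Spawned butterflies are tracked and destroyed when the item dropper resets or play ends.
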(event Custom|on%20fodder%20death
  (bind _returnvalue (Transformation|GetActorLocation))
  (bind _returnvalue_2 (Transformation|GetActorLocation))
  (switch Utilities|FlowControl|Switch|SwitchonAICharacter_States (Variables|/Game/SpyroContent/Global_Assets/Global_Components/Base_AI_Character.Base_AI_Character_C|GetAICharacter_State (Variables|Default|GetWalking_AI_Character))
    (:NewEnumerator3
      (bind _asspyro_save_data (CallFunction|LoadSpyroGame self))
      (bind _difficulty (CallFunction|ConvertSkillLevelFloattoEnum (Variables|/Game/SpyroContent/Global_Assets/Global_SaveData/Spyro_SaveData.Spyro_SaveData_C|GetSkill_Level _asspyro_save_data)))
      (bind _asspyro_universal_save_data (CallFunction|LoadUniversalSave))
      (if (or (and (or (Utilities|Enum|Equal(Enum) (Variables|/Game/SpyroContent/Global_Assets/Global_SaveData/Spyro_Universal_Save_Data.Spyro_Universal_Save_Data_C|GetDifficulty _asspyro_universal_save_data) "NewEnumerator0") (and (Utilities|Enum|Equal(Enum) (Variables|/Game/SpyroContent/Global_Assets/Global_SaveData/Spyro_Universal_Save_Data.Spyro_Universal_Save_Data_C|GetDifficulty _asspyro_universal_save_data) "NewEnumerator4") (Utilities|Enum|Equal(Enum) _difficulty "NewEnumerator0"))) (Math|Random|RandomBoolwithWeight 0.1)) (and (or (Utilities|Enum|Equal(Enum) (Variables|/Game/SpyroContent/Global_Assets/Global_SaveData/Spyro_Universal_Save_Data.Spyro_Universal_Save_Data_C|GetDifficulty _asspyro_universal_save_data) "NewEnumerator1") (and (Utilities|Enum|Equal(Enum) (Variables|/Game/SpyroContent/Global_Assets/Global_SaveData/Spyro_Universal_Save_Data.Spyro_Universal_Save_Data_C|GetDifficulty _asspyro_universal_save_data) "NewEnumerator4") (Utilities|Enum|Equal(Enum) _difficulty "NewEnumerator1"))) (Math|Random|RandomBoolwithWeight 0.05)))
        (bind _returnvalue_3 (Game|SpawnActorfromClass "/Game/SpyroContent/Global_Assets/Global_Level_Items/Butterflies/Actors/Butterfly_BP.Butterfly_BP_C" (Math|Transform|MakeTransform (Math|Vector|MakeVector (+ (.x _returnvalue_2) 1e+01) (+ (.y _returnvalue_2) 1e+01) (.z _returnvalue_2)) "0, 0, 0" "1,1,1") "AdjustIfPossibleButAlwaysSpawn" 0 0))
        (Utilities|Array|Add (Variables|Default|GetLucky%20Butterflies) _returnvalue_3)
        (bind _returnvalue_4 (Game|SpawnActorfromClass "/Game/SpyroContent/Global_Assets/Global_Level_Items/Butterflies/Actors/Butterfly_BP.Butterfly_BP_C" (Math|Transform|MakeTransform (Math|Vector|MakeVector (+ (.x _returnvalue) -1e+01) (+ (.y _returnvalue) -1e+01) (.z _returnvalue)) "0, 0, 0" "1,1,1") "AdjustIfPossibleButAlwaysSpawn" 0 0))
        (Utilities|Array|Add (Variables|Default|GetLucky%20Butterflies) _returnvalue_4)))))

(event Custom|clear%20lucky%20butterflies
  (for _array_element (Variables|Default|GetLucky%20Butterflies)
    (Utilities|IsValid _array_element
      (:Is%20Valid
        (Actor|DestroyActor _array_element)))))

(event EventBeginPlay
  (|CallParentFunction)
  (EventDispatchers|BindEventtoMyStateChanged (Variables|Default|GetWalking_AI_Character) (delegate Custom|on%20fodder%20death))
  (EventDispatchers|BindEventtoItemDropperSuccessfullyReset (Variables|Default|GetDrops_Items) (delegate Custom|clear%20lucky%20butterflies)))

(event EventEndPlay
  (params (EndPlayReason :type EEndPlayReason%20Enum :default "Destroyed"))
  (|CallParentFunction EndPlayReason)
  (for _array_element (Variables|Default|GetLucky%20Butterflies)
    (Utilities|IsValid _array_element
      (:Is%20Valid
        (Actor|DestroyActor _array_element)))))

(fn ConstructionScript
  (|CallParentFunction))