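; Swimming frog fodder character, a child Blueprint of an AI character with walking AI and damageable behavior.
; On BeginPlay it assigns its Hitbox to the Damageable component and listens for AI state changes.
; Each state change toggles CharacterMovement gravity, enabling it only in one specific AI state and leaving the frog weightless in all others.
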(event Custom|on%20swimming%20frogs%20state%20changed
  (Variables|/Script/Engine.CharacterMovementComponent|SetGravityScale (Variables|Character|GetCharacterMovement) (select (Utilities|Enum|Equal(Enum) (Variables|/Game/SpyroContent/Global_Assets/Global_Components/Base_AI_Character.Base_AI_Character_C|GetAICharacter_State (Variables|Default|GetWalking_AI_Character)) "NewEnumerator3") 1.0 0.0)))

(event EventBeginPlay
  (|CallParentFunction)
  (EventDispatchers|BindEventtoMyStateChanged (Variables|Default|GetWalking_AI_Character) (delegate Custom|on%20swimming%20frogs%20state%20changed))
  (Variables|/Game/SpyroContent/Global_Assets/Global_Components/Damageable_Com.Damageable_Com_C|SetObject's%20Hitbox%20Component (Variables|Default|GetDamageable) (Variables|Default|GetHitbox)))

(fn ConstructionScript
  (|CallParentFunction))