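; Fodder Blueprint, apparently a base class, for AI characters that flee from the nearest player they are alert to.
; While Alert with Runs Away behavior, Tick walks it forward and smoothly turns its yaw away from that player, plus a random offset from the WalkingAICharacter.
; A stuck-prevention timer starts on state change; when stuck, the fodder snaps 110 degrees to a random side and holds that heading for a second.
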(event Custom|Dont%20Run%20From%20Player%20for%20a%20Bit
  (Utilities|FlowControl|DoOnce false :!label _label
    (:Completed
      (Variables|Default|SetDont_Run_From_Player_for_a_Bit true)
      (Variables|Default|SetStuck%20on%20Wall%20Rotation (.yaw (Transformation|GetActorRotation)))
      (Variables|Default|SetPositive%20Unstuck (Math|Random|RandomBool))
      (Utilities|FlowControl|Delay 1.0)
      (Variables|Default|SetDont_Run_From_Player_for_a_Bit false)
      (goto _label Reset))))

(event Custom|Fodder%20Run%20Away
  (bind _stuck_on_wall_rotation (Variables|Default|GetStuck%20on%20Wall%20Rotation))
  (bind _positive_unstuck (Variables|Default|GetPositive%20Unstuck))
  (bind _walking_ai_character (Variables|Default|GetWalking_AI_Character))
  (bind _returnvalue (select _positive_unstuck 1.0 -1.0))
  (bind _returnvalue_2 (* 1.1e+02 _returnvalue))
  (bind _returnvalue_3 (+ _stuck_on_wall_rotation _returnvalue_2))
  (bind _returnvalue_4 (Math|Rotator|MakeRotator 0.0 0.0 _returnvalue_3))
  (Default|WalkForward _walking_ai_character)
  (bind _closest_player1 (Default|GetNearestPlayerImAlertto _walking_ai_character))
  (Utilities|IsValid _closest_player1
    (:Is%20Valid
      (if (Variables|Default|GetDont_Run_From_Player_for_a_Bit)
        (if (not (Math|Rotator|Equal(Rotator) (Transformation|GetActorRotation) _returnvalue_4 0.1))
          (Transformation|SetActorRotation _returnvalue_4))
        (elif (not (Math|Rotator|Equal(Rotator) (Transformation|GetActorRotation) (Math|Rotator|MakeRotator 0.0 0.0 (.yaw (Math|Rotator|Lerp(Rotator) (Transformation|GetActorRotation) (Math|Rotator|MakeRotator 0.0 0.0 (+ (.yaw (Math|Rotator|FindLookatRotation (Transformation|GetActorLocation) (Transformation|GetActorLocation _closest_player1))) (+ (Variables|/Game/SpyroContent/Global_Assets/Global_Components/Base_AI_Character.Base_AI_Character_C|GetRandom_RotationAmount (Variables|Default|GetWalking_AI_Character)) 1.8e+02))) (* (Utilities|Time|GetWorldDeltaSeconds) 1e+01) true))) 0.1))
          (Transformation|SetActorRotation (Math|Rotator|MakeRotator 0.0 0.0 (.yaw (Math|Rotator|Lerp(Rotator) (Transformation|GetActorRotation) (Math|Rotator|MakeRotator 0.0 0.0 (+ (.yaw (Math|Rotator|FindLookatRotation (Transformation|GetActorLocation) (Transformation|GetActorLocation _closest_player1))) (+ (Variables|/Game/SpyroContent/Global_Assets/Global_Components/Base_AI_Character.Base_AI_Character_C|GetRandom_RotationAmount (Variables|Default|GetWalking_AI_Character)) 1.8e+02))) (* (Utilities|Time|GetWorldDeltaSeconds) 1e+01) true)))))))))

(event Custom|On%20RunAway%20Fodder%20State%20Changed
  (bind _walking_ai_character (Variables|Default|GetWalking_AI_Character))
  (switch Utilities|FlowControl|Switch|SwitchonAICharacter_AlertBehaviors (Variables|/Game/SpyroContent/Global_Assets/Global_Components/Base_AI_Character.Base_AI_Character_C|GetAlert_Behavior (Variables|Default|GetWalking_AI_Character))
    (:NewEnumerator1
      (Default|StarttheStuckPreventionTimer _walking_ai_character 0.2)
      (if (not (Variables|/Game/SpyroContent/Global_Assets/Global_Components/Base_AI_Character.Base_AI_Character_C|GetRandomizingRotations _walking_ai_character))
        (Variables|/Game/SpyroContent/Global_Assets/Global_Components/Base_AI_Character.Base_AI_Character_C|SetRandom_RotationAmount _walking_ai_character 0.0)
        (Default|RandomRotation _walking_ai_character)))))

(event Custom|RunAway%20Fodder%20Stuck%20Prevention
  (bind _returnvalue (Default|IsThisActorStuck? (Variables|Default|GetWalking_AI_Character)))
  (if _returnvalue
    (CallFunction|DontRunfromPlayerforABit)))

(event EventTick
  (params (DeltaSeconds :type Float%20%28single-precision%29))
  (switch Utilities|FlowControl|Switch|SwitchonAICharacter_States (Variables|/Game/SpyroContent/Global_Assets/Global_Components/Base_AI_Character.Base_AI_Character_C|GetAICharacter_State (Variables|Default|GetWalking_AI_Character))
    (:NewEnumerator1
      (switch Utilities|FlowControl|Switch|SwitchonAICharacter_AlertBehaviors (Variables|/Game/SpyroContent/Global_Assets/Global_Components/Base_AI_Character.Base_AI_Character_C|GetAlert_Behavior (Variables|Default|GetWalking_AI_Character))
        (:NewEnumerator1
          (CallFunction|FodderRunAway))))))

(event EventBeginPlay
  (bind _walking_ai_character (Variables|Default|GetWalking_AI_Character))
  (|CallParentFunction)
  (EventDispatchers|BindEventtoMyStateChanged _walking_ai_character (delegate Custom|On%20RunAway%20Fodder%20State%20Changed))
  (CallFunction|OnRunAwayFodderStateChanged)
  (EventDispatchers|BindEventtoStuckPreventionWasChecked _walking_ai_character (delegate Custom|RunAway%20Fodder%20Stuck%20Prevention)))

(fn ConstructionScript
  (|CallParentFunction))

(fn CheckifFodderIsStuck
  (bind _returnvalue (Default|IsThisActorStuck? (Variables|Default|GetWalking_AI_Character)))
  (if _returnvalue
    (CallFunction|DontRunfromPlayerforABit)))