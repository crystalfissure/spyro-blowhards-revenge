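; Sheep fodder AI character that acts as a damageable critter, built on parent walking AI behavior.
; On begin play it registers its hitbox with the Damageable component and has a small random chance to use a black sheep material.
; It binds to the game instance's treasure-skin change event, then after a short delay sets its death scream based on the saved S1 treasure setting.
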(event EventBeginPlay
  (|CallParentFunction)
  (Variables|/Game/SpyroContent/Global_Assets/Global_Components/Damageable_Com.Damageable_Com_C|SetObject's%20Hitbox%20Component (Variables|Default|GetDamageable) (Variables|Default|GetHitbox))
  (if (Math|Random|RandomBoolwithWeight 0.1)
    (Rendering|Material|SetMaterial (Variables|Character|GetMesh) 0 "/Game/SpyroContent/Global_Assets/Global_Characters/AI_Characters/Actors/Fodder/Sheep/Materials/black_sheep_mat.black_sheep_mat"))
  (bind _asspyro_persistant_data (Utilities|Casting|CastToSpyro_PersistantData (Game|GetGameInstance)))
  (EventDispatchers|BindEventtoChangeTreasureSkins _asspyro_persistant_data (delegate S1DeathScream))
  (Utilities|FlowControl|Delay 0.2)
  (CallFunction|SetDeathScream))

(event EventTick
  (params (DeltaSeconds :type Float%20%28single-precision%29)))

(fn ConstructionScript
  (|CallParentFunction))

(event Custom|Set%20Death%20Scream
  (bind _asspyro_save_data (CallFunction|LoadSpyroGame self))
  (Utilities|IsValid _asspyro_save_data
    (:Is%20Valid
      (Variables|/Game/SpyroContent/Global_Assets/Global_Components/Base_AI_Character.Base_AI_Character_C|SetDeath_Scream (Variables|Default|GetWalking_AI_Character) (select (Variables|/Game/SpyroContent/Global_Assets/Global_SaveData/Spyro_SaveData.Spyro_SaveData_C|GetS1_Treasure _asspyro_save_data) 0 "/Game/SpyroContent/Global_Assets/Global_Characters/AI_Characters/Actors/Fodder/Sheep/Audio/SheepHit1.SheepHit1")))))