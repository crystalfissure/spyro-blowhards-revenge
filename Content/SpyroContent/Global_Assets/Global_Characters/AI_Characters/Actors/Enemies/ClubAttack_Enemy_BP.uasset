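; Club-attack enemy Blueprint that extends a parent enemy class with a range check for leaving one of its AI states.
; Each Tick, while its walking AI character is in that state, it measures the distance to the nearest player it is alert to.
; When that distance exceeds the attack sphere radius plus the player's capsule radius, it switches to another state.
; The construction script only calls the parent.
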(event EventTick
  (params (DeltaSeconds :type Float%20%28single-precision%29))
  (|CallParentFunction DeltaSeconds)
  (if (Utilities|Enum|Equal(Enum) (Variables|/Game/SpyroContent/Global_Assets/Global_Components/Base_AI_Character.Base_AI_Character_C|GetAICharacter_State (Variables|Default|GetWalking_AI_Character)) "NewEnumerator2")
    (bind _closest_player1 (Default|GetNearestPlayerImAlertto (Variables|Default|GetWalking_AI_Character)))
    (if (> (Transformation|GetDistanceTo _closest_player1 self) (+ (Variables|/Script/Engine.SphereComponent|GetSphereRadius (Variables|Default|GetAttack_Radius)) (Variables|/Script/Engine.CapsuleComponent|GetCapsuleRadius (Variables|/Script/Engine.Character|GetCapsuleComponent _closest_player1))))
      (Default|ChangeAICharacterState (Variables|Default|GetWalking_AI_Character) "NewEnumerator1"))))

(fn ConstructionScript
  (|CallParentFunction))