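; Plane Thief enemy that flies a looping spline, reversing when the player overlaps its front or back trigger.
; Tick advances it while Attacking, or until it nears the spline start, at a difficulty-based speed.
; A looping timer lowers player skill during Attacking.
; Death spawns a dummy thief and basket burst, then calls PlaneThiefDestroyed; the Spyro 1 treasure-skin setting swaps its sounds.
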(event OnComponentBeginOverlap(Front_Trigger)
  (params (OverlappedComponent :type Primitive%20Component%20Object%20Reference) (OtherActor :type Actor%20Object%20Reference) (OtherComp :type Primitive%20Component%20Object%20Reference) (OtherBodyIndex :type Integer) (bFromSweep :type Boolean) (SweepResult :type Hit%20Result%20Structure%20%28by%20ref%29))
  (bind _asbp_base_playable (Utilities|Casting|CastToBP_Base_Playable OtherActor))
  (if (and (== (Variables|/Script/Engine.Character|GetCapsuleComponent _asbp_base_playable) OtherComp) (not (Variables|Default|GetFly%20Clockwise)))
    (Variables|Default|SetFly%20Clockwise true)
    (Transformation|SetRelativeRotation (Variables|Character|GetMesh) (Math|Rotator|MakeRotator 0.0 0.0 (select (Variables|Default|GetFly%20Clockwise) 9e+01 -9e+01)) false false)))

(event OnComponentBeginOverlap(Back_Trigger)
  (params (OverlappedComponent :type Primitive%20Component%20Object%20Reference) (OtherActor :type Actor%20Object%20Reference) (OtherComp :type Primitive%20Component%20Object%20Reference) (OtherBodyIndex :type Integer) (bFromSweep :type Boolean) (SweepResult :type Hit%20Result%20Structure%20%28by%20ref%29))
  (bind _asbp_base_playable (Utilities|Casting|CastToBP_Base_Playable OtherActor))
  (if (and (== (Variables|/Script/Engine.Character|GetCapsuleComponent _asbp_base_playable) OtherComp) (Variables|Default|GetFly%20Clockwise))
    (Variables|Default|SetFly%20Clockwise false)
    (Transformation|SetRelativeRotation (Variables|Character|GetMesh) (Math|Rotator|MakeRotator 0.0 0.0 (select (Variables|Default|GetFly%20Clockwise) 9e+01 -9e+01)) false false)))

(event Custom|On%20State%20Change
  (switch Utilities|FlowControl|Switch|SwitchonAICharacter_States (Variables|/Game/SpyroContent/Global_Assets/Global_Components/Base_AI_Character.Base_AI_Character_C|GetAICharacter_State (Variables|Default|GetWalking_AI_Character))
    (:NewEnumerator3
      (Audio|Components|Audio|Stop (Variables|Default|GetAudio))
      (Game|SpawnActorfromClass "/Game/SpyroContent/Global_Assets/Global_Characters/AI_Characters/Actors/Enemies/Thief/Animations/DummyThief_BP.DummyThief_BP_C" (Transformation|GetActorTransform) "AlwaysSpawn" 0 0)
      (if (Variables|Default|GetS1%20Mode)
        (Audio|PlaySoundatLocation "/Game/SpyroContent/Global_Assets/Global_Characters/AI_Characters/Actors/Enemies/Thief/Audio/EggThiefHitGrnd1.EggThiefHitGrnd1" (Transformation|GetActorLocation) "0, 0, 0" 2.0 1.0 0.0 "/Game/SpyroContent/Global_Assets/Global_Audio/Attenuation/Spyro_Attenuation_Even_Farther.Spyro_Attenuation_Even_Farther" 0 0))
      (bind _returnvalue (Game|SpawnActorfromClass "/Game/SpyroContent/Global_Assets/Global_Level_Items/Treasure_Containers/Basket/Actors/Basket_Burst_BP.Basket_Burst_BP_C" (Transformation|GetActorTransform) "AlwaysSpawn" 0 0))
      (Default|ShardBurstAction _returnvalue "/Game/SpyroContent/Global_Assets/Global_Level_Items/Treasure_Containers/Metal_Chest/Meshes/metal_chest_shard.metal_chest_shard" "/Game/SpyroContent/Global_Assets/Global_Level_Items/Treasure_Containers/Metal_Chest/Meshes/metal_chest_shard_2.metal_chest_shard_2")
      (Utilities|FlowControl|Delay 1.0)
      (Default|CallPlaneThiefDestroyed))))

(event Custom|S1%20Mode%20Toggle
  (Variables|Default|SetS1%20Mode (not (Variables|Default|GetS1%20Mode)))
  (Variables|/Game/SpyroContent/Global_Assets/Global_Components/Base_AI_Character.Base_AI_Character_C|SetDeath_Scream (Variables|Default|GetWalking_AI_Character) (select (Variables|Default|GetS1%20Mode) "/Game/SpyroContent/Global_Assets/Global_Level_Items/Treasure_Containers/Chest/ChestBreak1.ChestBreak1" "/Game/SpyroContent/Global_Assets/Global_Characters/AI_Characters/Actors/Enemies/Plane_Thief/Audio/plane_thief_explosion.plane_thief_explosion"))
  (Audio|Components|Audio|SetSound (Variables|Default|GetAudio) (select (Variables|Default|GetS1%20Mode) "/Game/SpyroContent/Global_Assets/Global_Characters/AI_Characters/Actors/Enemies/Plane_Thief/Audio/plane_thief_propeller.plane_thief_propeller" "/Game/SpyroContent/Global_Assets/Global_Characters/AI_Characters/Actors/Enemies/Plane_Thief/Audio/plane_thief_yotd.plane_thief_yotd")))

(event EventSetMyDifficulty
  (bind _medium_walk_speed (Variables|Default|GetMedium%20Walk%20Speed))
  (bind _medium_walk_speed_2 (Variables|Default|GetMedium%20Walk%20Speed))
  (|CallParentFunction)
  (bind _asspyro_universal_save_data (CallFunction|LoadUniversalSave))
  (if (Utilities|Enum|Equal(Enum) (Variables|/Game/SpyroContent/Global_Assets/Global_SaveData/Spyro_Universal_Save_Data.Spyro_Universal_Save_Data_C|GetDifficulty _asspyro_universal_save_data) "NewEnumerator4")
    (bind _asspyro_save_data (CallFunction|LoadSpyroGame self))
    (bind _difficulty (CallFunction|ConvertSkillLevelFloattoEnum (Variables|/Game/SpyroContent/Global_Assets/Global_SaveData/Spyro_SaveData.Spyro_SaveData_C|GetSkill_Level _asspyro_save_data)))
    (Variables|Default|SetPlane%20Speed (Utilities|Select :Index _difficulty :NewEnumerator4 _medium_walk_speed_2 :NewEnumerator0 (Variables|Default|GetEasy%20Walk%20Speed) :NewEnumerator1 _medium_walk_speed_2 :NewEnumerator2 (Variables|Default|GetHard%20Walk%20Speed) :NewEnumerator3 (Variables|Default|GetNightmare%20Walk%20Speed)))
    (else
      (Variables|Default|SetPlane%20Speed (Utilities|Select :Index (Variables|/Game/SpyroContent/Global_Assets/Global_SaveData/Spyro_Universal_Save_Data.Spyro_Universal_Save_Data_C|GetDifficulty _asspyro_universal_save_data) :NewEnumerator4 _medium_walk_speed :NewEnumerator0 (Variables|Default|GetEasy%20Walk%20Speed) :NewEnumerator1 _medium_walk_speed :NewEnumerator2 (Variables|Default|GetHard%20Walk%20Speed) :NewEnumerator3 (Variables|Default|GetNightmare%20Walk%20Speed))))))

(event EventBeginPlay
  (bind _spline (Variables|Default|GetSpline))
  (bind _spline_2 (Variables|Default|GetSpline))
  (bind _returnvalue (Spline|GetTransformatDistanceAlongSpline _spline_2 0.0 "World" false))
  (|CallParentFunction)
  (bind _output_get (Variables|Default|SetSpline%20Transform (Transformation|GetWorldTransform (Variables|Default|GetSpline))))
  (Utilities|Time|SetTimerbyFunctionName 0 "Drain Player's Skill" 1.0 true)
  (Transformation|SetAbsolute _spline true true true)
  (Transformation|SetWorldTransform _spline _output_get false false)
  (Transformation|SetActorLocationAndRotation (.location _returnvalue) (.rotation _returnvalue))
  (EventDispatchers|BindEventtoMyStateChanged (Variables|Default|GetWalking_AI_Character) (delegate Custom|On%20State%20Change))
  (bind _asspyro_persistant_data (Utilities|Casting|CastToSpyro_PersistantData (Game|GetGameInstance))
    (:then
      (EventDispatchers|BindEventtoChangeTreasureSkins _asspyro_persistant_data (delegate Custom|S1%20Mode%20Toggle)))
    (:CastFailed
      _))
  (bind _asspyro_save_data (CallFunction|LoadSpyroGame self))
  (Variables|Default|SetS1%20Mode (Variables|/Game/SpyroContent/Global_Assets/Global_SaveData/Spyro_SaveData.Spyro_SaveData_C|GetS1_Treasure _asspyro_save_data))
  (Variables|/Game/SpyroContent/Global_Assets/Global_Components/Base_AI_Character.Base_AI_Character_C|SetDeath_Scream (Variables|Default|GetWalking_AI_Character) (select (Variables|Default|GetS1%20Mode) "/Game/SpyroContent/Global_Assets/Global_Level_Items/Treasure_Containers/Chest/ChestBreak1.ChestBreak1" "/Game/SpyroContent/Global_Assets/Global_Characters/AI_Characters/Actors/Enemies/Plane_Thief/Audio/plane_thief_explosion.plane_thief_explosion"))
  (Audio|Components|Audio|SetSound (Variables|Default|GetAudio) (select (Variables|Default|GetS1%20Mode) "/Game/SpyroContent/Global_Assets/Global_Characters/AI_Characters/Actors/Enemies/Plane_Thief/Audio/plane_thief_propeller.plane_thief_propeller" "/Game/SpyroContent/Global_Assets/Global_Characters/AI_Characters/Actors/Enemies/Plane_Thief/Audio/plane_thief_yotd.plane_thief_yotd")))

(event EventTick
  (params (DeltaSeconds :type Float%20%28single-precision%29))
  (bind _spline (Variables|Default|GetSpline))
  (bind _returnvalue (Spline|GetSplineLength _spline))
  (|CallParentFunction DeltaSeconds)
  (if (and (or (Utilities|Enum|Equal(Enum) (Variables|/Game/SpyroContent/Global_Assets/Global_Components/Base_AI_Character.Base_AI_Character_C|GetAICharacter_State (Variables|Default|GetWalking_AI_Character)) "NewEnumerator2") (not (Math|Float|InRange(Float) (Variables|Default|GetDistance) -1e+02 1e+02))) (not (Utilities|Enum|Equal(Enum) (Variables|/Game/SpyroContent/Global_Assets/Global_Components/Base_AI_Character.Base_AI_Character_C|GetAICharacter_State (Variables|Default|GetWalking_AI_Character)) "NewEnumerator3")))
    (Variables|Default|SetDistance (select (> (+ (* DeltaSeconds (* (Variables|Default|GetPlane%20Speed) (select (Variables|Default|GetFly%20Clockwise) -1.0 1.0))) (Variables|Default|GetDistance)) _returnvalue) 0.0 (select (< (+ (* DeltaSeconds (* (Variables|Default|GetPlane%20Speed) (select (Variables|Default|GetFly%20Clockwise) -1.0 1.0))) (Variables|Default|GetDistance)) 0.0) _returnvalue (+ (* DeltaSeconds (* (Variables|Default|GetPlane%20Speed) (select (Variables|Default|GetFly%20Clockwise) -1.0 1.0))) (Variables|Default|GetDistance)))))
    (Transformation|SetActorLocationAndRotation (.location (Spline|GetTransformatDistanceAlongSpline (Variables|Default|GetSpline) (Variables|Default|GetDistance) "World" false)) (.rotation (Spline|GetTransformatDistanceAlongSpline (Variables|Default|GetSpline) (Variables|Default|GetDistance) "World" false)))))

(fn ConstructionScript
  (|CallParentFunction))

(fn DrainPlayer'sSkill
  (if (Utilities|Enum|Equal(Enum) (Variables|/Game/SpyroContent/Global_Assets/Global_Components/Base_AI_Character.Base_AI_Character_C|GetAICharacter_State (Variables|Default|GetWalking_AI_Character)) "NewEnumerator2")
    (CallFunction|UpdateSkillLevel (* (Variables|Default|GetSkill%20Level%20Penalty) -1.0) self)))