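; Runaway thief enemy that flees along its own world-locked spline, draining the player's skill level while active.
; Tick snaps it to the nearest spline point and drives it along the tangent, while detection boxes flip direction when the nearest alerted player overlaps.
; Forward traces and falling checks launch it over walls and ledges, and floor traces tilt the mesh.
; Difficulty sets run speed, and a gem reset returns it to its start.
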(event OnComponentBeginOverlap(Running_Front_Detection_Box)
  (params (OverlappedComponent :type Primitive%20Component%20Object%20Reference) (OtherActor :type Actor%20Object%20Reference) (OtherComp :type Primitive%20Component%20Object%20Reference) (OtherBodyIndex :type Integer) (bFromSweep :type Boolean) (SweepResult :type Hit%20Result%20Structure%20%28by%20ref%29))
  (bind _returnvalue (CallFunction|ShouldThisOverlapChangeThief'sDirection? OtherActor OtherComp))
  (if (and _returnvalue (Utilities|Enum|Equal(Enum) (Variables|/Game/SpyroContent/Global_Assets/Global_Components/Base_AI_Character.Base_AI_Character_C|GetAICharacter_State (Variables|Default|GetWalking_AI_Character)) "NewEnumerator2"))
    (CallFunction|RunningDirectionChanged)))

(event OnComponentEndOverlap(Unattack_Radius)
  (params (OverlappedComponent :type Primitive%20Component%20Object%20Reference) (OtherActor :type Actor%20Object%20Reference) (OtherComp :type Primitive%20Component%20Object%20Reference) (OtherBodyIndex :type Integer))
  (bind _asbp_base_playable (Utilities|Casting|CastToBP_Base_Playable OtherActor))
  (if (and (== (Variables|/Script/Engine.Character|GetCapsuleComponent _asbp_base_playable) OtherComp) (Utilities|Enum|Equal(Enum) (Variables|/Game/SpyroContent/Global_Assets/Global_Components/Base_AI_Character.Base_AI_Character_C|GetAICharacter_State (Variables|Default|GetWalking_AI_Character)) "NewEnumerator2"))
    (Default|ChangeAICharacterState (Variables|Default|GetWalking_AI_Character) "NewEnumerator1")))

(event OnComponentBeginOverlap(NotRunning_Front_Detection_Box)
  (params (OverlappedComponent :type Primitive%20Component%20Object%20Reference) (OtherActor :type Actor%20Object%20Reference) (OtherComp :type Primitive%20Component%20Object%20Reference) (OtherBodyIndex :type Integer) (bFromSweep :type Boolean) (SweepResult :type Hit%20Result%20Structure%20%28by%20ref%29))
  (bind _returnvalue (CallFunction|ShouldThisOverlapChangeThief'sDirection? OtherActor OtherComp))
  (if (and _returnvalue (not (Utilities|Enum|Equal(Enum) (Variables|/Game/SpyroContent/Global_Assets/Global_Components/Base_AI_Character.Base_AI_Character_C|GetAICharacter_State (Variables|Default|GetWalking_AI_Character)) "NewEnumerator2")))
    (CallFunction|RunningDirectionChanged)))

(event OnComponentEndOverlap(Running_Front_Detection_Box)
  (params (OverlappedComponent :type Primitive%20Component%20Object%20Reference) (OtherActor :type Actor%20Object%20Reference) (OtherComp :type Primitive%20Component%20Object%20Reference) (OtherBodyIndex :type Integer))
  (bind _returnvalue (CallFunction|ShouldThisOverlapChangeThief'sDirection? OtherActor OtherComp))
  ;[1 1 1] it seems this should just stay unplugged?
  (if (and _returnvalue false)
    _))

(event OnComponentEndOverlap(NotRunning_Front_Detection_Box)
  (params (OverlappedComponent :type Primitive%20Component%20Object%20Reference) (OtherActor :type Actor%20Object%20Reference) (OtherComp :type Primitive%20Component%20Object%20Reference) (OtherBodyIndex :type Integer))
  (bind _returnvalue (CallFunction|ShouldThisOverlapChangeThief'sDirection? OtherActor OtherComp))
  (if (and _returnvalue (not (Utilities|Enum|Equal(Enum) (Variables|/Game/SpyroContent/Global_Assets/Global_Components/Base_AI_Character.Base_AI_Character_C|GetAICharacter_State (Variables|Default|GetWalking_AI_Character)) "NewEnumerator2")))
    (CallFunction|RunningDirectionChanged)))

(event Custom|On%20State%20Change
  (if (Utilities|Enum|Equal(Enum) (Variables|/Game/SpyroContent/Global_Assets/Global_Components/Base_AI_Character.Base_AI_Character_C|GetAICharacter_State (Variables|Default|GetWalking_AI_Character)) "NewEnumerator3")
    (Variables|Default|SetRunning%20Clockwise false)))

(event Custom|Unlock%20Run%20Other%20Way
  (Utilities|FlowControl|Delay (Variables|Default|GetTurnaround%20Lock%20Duration))
  (Variables|Default|SetTurnaround%20Lock false)
  (Variables|/Script/Engine.CharacterMovementComponent|SetMaxWalkSpeed (Variables|Character|GetCharacterMovement) (Variables|Default|GetDefault%20Walk%20Speed)))

(event Custom|Return%20to%20Spline
  (Variables|Default|SetRunning%20Clockwise false)
  (Transformation|SetActorTransform (Variables|Default|GetRunAway_Enemy_DefaultTransform)))

(event EventSetMyDifficulty
  (bind _medium_walk_speed (Variables|Default|GetMedium%20Walk%20Speed))
  (bind _medium_walk_speed_2 (Variables|Default|GetMedium%20Walk%20Speed))
  (|CallParentFunction)
  (bind _asspyro_universal_save_data (CallFunction|LoadUniversalSave))
  (if (Utilities|Enum|Equal(Enum) (Variables|/Game/SpyroContent/Global_Assets/Global_SaveData/Spyro_Universal_Save_Data.Spyro_Universal_Save_Data_C|GetDifficulty _asspyro_universal_save_data) "NewEnumerator4")
    (bind _asspyro_save_data (CallFunction|LoadSpyroGame self))
    (bind _difficulty (CallFunction|ConvertSkillLevelFloattoEnum (Variables|/Game/SpyroContent/Global_Assets/Global_SaveData/Spyro_SaveData.Spyro_SaveData_C|GetSkill_Level _asspyro_save_data)))
    (Variables|/Script/Engine.CharacterMovementComponent|SetMaxWalkSpeed (Variables|Character|GetCharacterMovement) (Utilities|Select :Index _difficulty :NewEnumerator4 _medium_walk_speed :NewEnumerator0 (Variables|Default|GetEasy%20Walk%20Speed) :NewEnumerator1 _medium_walk_speed :NewEnumerator2 (Variables|Default|GetHard%20Walk%20Speed) :NewEnumerator3 (Variables|Default|GetNightmare%20Walk%20Speed)))
    (Variables|Default|SetDefault%20Walk%20Speed (Utilities|Select :Index _difficulty :NewEnumerator4 _medium_walk_speed :NewEnumerator0 (Variables|Default|GetEasy%20Walk%20Speed) :NewEnumerator1 _medium_walk_speed :NewEnumerator2 (Variables|Default|GetHard%20Walk%20Speed) :NewEnumerator3 (Variables|Default|GetNightmare%20Walk%20Speed)))
    (else
      (Variables|/Script/Engine.CharacterMovementComponent|SetMaxWalkSpeed (Variables|Character|GetCharacterMovement) (Utilities|Select :Index (Variables|/Game/SpyroContent/Global_Assets/Global_SaveData/Spyro_Universal_Save_Data.Spyro_Universal_Save_Data_C|GetDifficulty _asspyro_universal_save_data) :NewEnumerator4 _medium_walk_speed_2 :NewEnumerator0 (Variables|Default|GetEasy%20Walk%20Speed) :NewEnumerator1 _medium_walk_speed_2 :NewEnumerator2 (Variables|Default|GetHard%20Walk%20Speed) :NewEnumerator3 (Variables|Default|GetNightmare%20Walk%20Speed)))
      (Variables|Default|SetDefault%20Walk%20Speed (Utilities|Select :Index (Variables|/Game/SpyroContent/Global_Assets/Global_SaveData/Spyro_Universal_Save_Data.Spyro_Universal_Save_Data_C|GetDifficulty _asspyro_universal_save_data) :NewEnumerator4 _medium_walk_speed_2 :NewEnumerator0 (Variables|Default|GetEasy%20Walk%20Speed) :NewEnumerator1 _medium_walk_speed_2 :NewEnumerator2 (Variables|Default|GetHard%20Walk%20Speed) :NewEnumerator3 (Variables|Default|GetNightmare%20Walk%20Speed))))))

(event EventBeginPlay
  (bind _spline (Variables|Default|GetSpline))
  (bind _capsulecomponent (Variables|Default|GetCapsuleComponent))
  (|CallParentFunction)
  (Utilities|Time|SetTimerbyFunctionName 0 "Drain Player's Skill" 1.0 true)
  (bind _output_get (Variables|Default|SetSpline%20Transform (Transformation|GetWorldTransform (Variables|Default|GetSpline))))
  (Transformation|SetAbsolute _spline true true true)
  (Transformation|SetWorldTransform _spline _output_get false false)
  (EventDispatchers|BindEventtoMyStateChanged (Variables|Default|GetWalking_AI_Character) (delegate Custom|On%20State%20Change))
  (bind _asspyro_persistant_data (Utilities|Casting|CastToSpyro_PersistantData (Game|GetGameInstance))
    (:then
      (EventDispatchers|BindEventtoResetGems _asspyro_persistant_data (delegate Custom|Return%20to%20Spline)))
    (:CastFailed
      _))
  (Utilities|FlowControl|Delay 0.2)
  (Transformation|SetWorldLocation _capsulecomponent (Spline|FindLocationClosesttoWorldLocation (Variables|Default|GetSpline) (Transformation|GetWorldLocation _capsulecomponent) "World") false false)
  (Variables|Default|SetRunAway_Enemy_DefaultTransform (Transformation|GetActorTransform)))

(event EventAttackRadiusOverlapped
  ;[1 1 1] im turning off the turnaround lock for now so he can change direction instantly no matter what. hopefully this doesnt cause any issues!
  (|CallParentFunction)
  (if (Variables|Default|GetUse%20the%20Turnaround%20Lock)
    (Variables|Default|SetTurnaround%20Lock true))
  (CallFunction|UnlockRunOtherWay))

(event EventTick
  (params (DeltaSeconds :type Float%20%28single-precision%29))
  (bind _capsulecomponent (Variables|Default|GetCapsuleComponent))
  (bind _walking_ai_character (Variables|Default|GetWalking_AI_Character))
  (bind _spline (Variables|Default|GetSpline))
  (bind _capsulecomponent_2 (Variables|Default|GetCapsuleComponent))
  (bind _spline_2 (Variables|Default|GetSpline))
  (bind _returnvalue (Transformation|GetWorldLocation _capsulecomponent))
  (bind _returnvalue_2 (Transformation|GetWorldLocation _capsulecomponent_2))
  (bind _returnvalue_3 (Class|SplineComponent|FindTangentClosesttoWorldLocation _spline _returnvalue "World"))
  (bind _returnvalue_4 (Spline|FindLocationClosesttoWorldLocation _spline_2 _returnvalue_2 "World"))
  (|CallParentFunction DeltaSeconds)
  (|ManageMeshRotation
    (:then_1
      (|ManageJumpOffLedges
        (:then_1
          (if (or (and (Utilities|Enum|Equal(Enum) (Variables|/Game/SpyroContent/Global_Assets/Global_Components/Base_AI_Character.Base_AI_Character_C|GetAICharacter_State _walking_ai_character) "NewEnumerator2") (Utilities|Enum|Equal(Enum) (Variables|/Game/SpyroContent/Global_Assets/Global_Components/Base_AI_Character.Base_AI_Character_C|GetAttack_Behavior _walking_ai_character) "NewEnumerator1")) (and (AI|Components|NavMovement|IsFalling (Variables|Character|GetCharacterMovement)) (not (Utilities|Enum|Equal(Enum) (Variables|/Game/SpyroContent/Global_Assets/Global_Components/Base_AI_Character.Base_AI_Character_C|GetAICharacter_State (Variables|Default|GetWalking_AI_Character)) "NewEnumerator3"))))
            (bind _outhit_bblockinghit (|LineTraceFromMeshsForward))
            (if _outhit_bblockinghit
              (if (Utilities|Time|IsValidTimerHandle (Variables|Default|GetWall%20Jump%20Timer))
                _
                (else
                  (bind _returnvalue_5 (Utilities|Time|SetTimerbyFunctionName 0 "Jump Over Wall" 0.2 true))
                  (Variables|Default|SetWall%20Jump%20Timer _returnvalue_5)))
              (else
                (CallFunction|StopWallJumpTimer)))
            (Transformation|SetWorldLocation (Variables|Default|GetCapsuleComponent) (Math|Vector|MakeVector (.x _returnvalue_4) (.y _returnvalue_4) (.z (Transformation|GetActorLocation))) true false)
            (Pawn|Input|AddMovementInput (select (Variables|Default|GetRunning%20Clockwise) (* _returnvalue_3 -1.0) _returnvalue_3) 1.0 true)
            (else
              (CallFunction|StopWallJumpTimer))))))))

(fn ConstructionScript
  (|CallParentFunction))

(fn JumpOverWall
  (bind _returnvalue (Transformation|GetActorForwardVector))
  (bind _returnvalue_2 (* _returnvalue 1.0))
  (if (not (Utilities|Enum|Equal(Enum) (Variables|/Game/SpyroContent/Global_Assets/Global_Components/Base_AI_Character.Base_AI_Character_C|GetAICharacter_State (Variables|Default|GetWalking_AI_Character)) "NewEnumerator3"))
    (Character|LaunchCharacter (Math|Vector|MakeVector (.x _returnvalue_2) (.y _returnvalue_2) (+ (.z _returnvalue_2) 8e+02)) false true)
    (Development|PrintString "thief launched")))

(fn StopWallJumpTimer
  (if (Utilities|Time|IsValidTimerHandle (Variables|Default|GetWall%20Jump%20Timer))
    (Utilities|Time|ClearandInvalidateTimerbyHandle (Variables|Default|GetWall%20Jump%20Timer))))

(fn RunningDirectionChanged
  (if (not (Variables|Default|GetNever%20Turns%20Around))
    (Variables|Default|SetRunning%20Clockwise (not (Variables|Default|GetRunning%20Clockwise)))
    (if (Variables|Default|GetUse%20the%20Turnaround%20Lock)
      (Variables|Default|SetTurnaround%20Lock true)
      (CallFunction|UnlockRunOtherWay))))

(fn ShouldThisOverlapChangeThief'sDirection?
  (params (Other%20Actor :type Object%20Object%20Reference) (Other%20Comp :type Object%20Object%20Reference))
  (bind _asbp_base_playable (Utilities|Casting|CastToBP_Base_Playable Other%20Actor)
    (:then
      (if (== (Variables|/Script/Engine.Character|GetCapsuleComponent _asbp_base_playable) Other%20Comp)
        (bind _closest_player1 (Default|GetNearestPlayerImAlertto (Variables|Default|GetWalking_AI_Character)))
        (LocalVariables|SetYes%20or%20No (Math|Boolean|ANDBoolean (== _closest_player1 _asbp_base_playable) (not (Utilities|Enum|Equal(Enum) (Variables|/Game/SpyroContent/Global_Assets/Global_Components/Base_AI_Character.Base_AI_Character_C|GetAICharacter_State (Variables|Default|GetWalking_AI_Character)) "NewEnumerator3")) (not (Variables|Default|GetTurnaround%20Lock))))
        (else
          (LocalVariables|SetYes%20or%20No false :!label _label))))
    (:CastFailed
      (goto _label)))
  (return (LocalVariables|GetYes%20or%20No)))

(fn LookatPlayer
  (bind _returnvalue (Math|Float|MakeLiteralFloat 0.1))
  (bind _walking_ai_character (Variables|Default|GetWalking_AI_Character))
  (bind _mesh (Variables|Character|GetMesh))
  (bind _mesh_2 (Variables|Character|GetMesh))
  (bind _returnvalue_2 (Transformation|GetWorldRotation _mesh_2))
  (bind _relativerotation (Variables|/Script/Engine.SceneComponent|GetRelativeRotation _mesh))
  (bind _aicharacter_state (Variables|/Game/SpyroContent/Global_Assets/Global_Components/Base_AI_Character.Base_AI_Character_C|GetAICharacter_State _walking_ai_character))
  (bind (_roll _pitch) (Math|Rotator|BreakRotator _returnvalue_2))
  (bind _returnvalue_3 (Math|Rotator|Lerp(Rotator) _relativerotation "0, 0, 0" _returnvalue true))
  (Utilities|FlowControl|Sequence
    (:then_0
      (if (and (or (and (> (Utilities|Array|Length (Variables|/Game/SpyroContent/Global_Assets/Global_Components/Base_AI_Character.Base_AI_Character_C|GetPlayers_I_Am_Alert_To (Variables|Default|GetWalking_AI_Character))) 0) (Utilities|Enum|Equal(Enum) _aicharacter_state "NewEnumerator1")) (and (Utilities|Enum|Equal(Enum) _aicharacter_state "NewEnumerator2") (Utilities|Enum|Equal(Enum) (Variables|/Game/SpyroContent/Global_Assets/Global_Components/Base_AI_Character.Base_AI_Character_C|GetAttack_Behavior _walking_ai_character) "NewEnumerator0"))) (not (AI|Components|NavMovement|IsFalling (Variables|Character|GetCharacterMovement))))
        (bind _closest_player1 (Default|GetNearestPlayerImAlertto (Variables|Default|GetWalking_AI_Character)))
        (if (not (Math|Rotator|Equal(Rotator) (Transformation|GetWorldRotation (Variables|Character|GetMesh)) (Math|Rotator|MakeRotator _roll _pitch (.yaw (Math|Rotator|Lerp(Rotator) _returnvalue_2 (Math|Rotator|MakeRotator _roll _pitch (.yaw (Math|Rotator|FindLookatRotation (Transformation|GetWorldLocation _mesh_2) (Transformation|GetActorLocation _closest_player1)))) _returnvalue true))) 0.1))
          (Transformation|SetWorldRotation (Variables|Character|GetMesh) (Math|Rotator|MakeRotator _roll _pitch (.yaw (Math|Rotator|Lerp(Rotator) _returnvalue_2 (Math|Rotator|MakeRotator _roll _pitch (.yaw (Math|Rotator|FindLookatRotation (Transformation|GetWorldLocation _mesh_2) (Transformation|GetActorLocation _closest_player1)))) _returnvalue true))) false false))
        (elif (not (Math|Rotator|Equal(Rotator) (Variables|/Script/Engine.SceneComponent|GetRelativeRotation (Variables|Character|GetMesh)) _returnvalue_3 0.1))
          (Transformation|SetRelativeRotation (Variables|Character|GetMesh) _returnvalue_3 false false))))
    (:then_1
      (return))))

(fn DrainPlayer'sSkill
  (if (Utilities|Enum|Equal(Enum) (Variables|/Game/SpyroContent/Global_Assets/Global_Components/Base_AI_Character.Base_AI_Character_C|GetAICharacter_State (Variables|Default|GetWalking_AI_Character)) "NewEnumerator2")
    (CallFunction|UpdateSkillLevel (* (Variables|Default|GetSkill%20Level%20Penalty) -1.0) self)))