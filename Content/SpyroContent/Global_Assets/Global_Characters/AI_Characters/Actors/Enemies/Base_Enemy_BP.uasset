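; Base enemy Blueprint for Spyro AI characters, handling attack triggering, player facing, difficulty and heated-metal feedback.
; Attack-radius overlaps and a looping sphere-trace ping move enemies into Attacking, gated by initial delay, cooldown and optional off-camera mercy.
; Tick turns enemies toward the nearest alerted player or back to their starting yaw.
; Saved settings or skill level set difficulty; timelines tint metal materials, and a timer repairs stuck frozen collision.
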(event OnComponentBeginOverlap(Attack_Radius)
  (params (OverlappedComponent :type Primitive%20Component%20Object%20Reference) (OtherActor :type Actor%20Object%20Reference) (OtherComp :type Primitive%20Component%20Object%20Reference) (OtherBodyIndex :type Integer) (bFromSweep :type Boolean) (SweepResult :type Hit%20Result%20Structure%20%28by%20ref%29))
  (Attacking|SomethingOverlappedAttackRadius OtherActor OtherComp))

(event Custom|On%20Enemy%20State%20Changed
  (switch Utilities|FlowControl|Switch|SwitchonAICharacter_States (Variables|/Game/SpyroContent/Global_Assets/Global_Components/Base_AI_Character.Base_AI_Character_C|GetAICharacter_State (Variables|Default|GetWalking_AI_Character))
    (:NewEnumerator0
      (Variables|Default|SetInitial%20Attack%20Delay true))
    (:NewEnumerator2
      (Utilities|Time|ClearandInvalidateTimerbyHandle (Variables|Attacking|GetAttack%20Cooldown%20Timer) :!label _label)
      (Variables|Attacking|SetCurrent_Cooldown_Time 0)
      (Variables|Difficulty|SetDamaged%20Player,%20Show%20Mercy false))
    (:NewEnumerator3
      (Variables|Default|SetInitial%20Attack%20Delay true)
      (goto _label))))

(event Custom|Set%20My%20Difficulty
  (bind _asspyro_universal_save_data (CallFunction|LoadUniversalSave))
  (if (Utilities|Enum|Equal(Enum) (Variables|/Game/SpyroContent/Global_Assets/Global_SaveData/Spyro_Universal_Save_Data.Spyro_Universal_Save_Data_C|GetDifficulty _asspyro_universal_save_data) "NewEnumerator4")
    (bind _asspyro_save_data (CallFunction|LoadSpyroGame self))
    (bind _difficulty (CallFunction|ConvertSkillLevelFloattoEnum (Variables|/Game/SpyroContent/Global_Assets/Global_SaveData/Spyro_SaveData.Spyro_SaveData_C|GetSkill_Level _asspyro_save_data)))
    (Variables|Difficulty|SetMy%20Current%20Difficulty _difficulty)
    (else
      (Variables|Difficulty|SetMy%20Current%20Difficulty (Variables|/Game/SpyroContent/Global_Assets/Global_SaveData/Spyro_Universal_Save_Data.Spyro_Universal_Save_Data_C|GetDifficulty _asspyro_universal_save_data)))))

(event Custom|Attack%20After%20Delay
  (if (Variables|Default|GetInitial%20Attack%20Delay)
    (Utilities|FlowControl|Delay (Variables|Default|GetAttack%20Delay))
    (Variables|Default|SetInitial%20Attack%20Delay false)
    (if (Utilities|Enum|Equal(Enum) (Variables|/Game/SpyroContent/Global_Assets/Global_Components/Base_AI_Character.Base_AI_Character_C|GetAICharacter_State (Variables|Default|GetWalking_AI_Character)) "NewEnumerator1")
      (bind _returnvalue (CallFunction|AmIonCamera? :!label _label))
      (if (or _returnvalue (not (Variables|Default|GetOff%20Camera%20Mercy)))
        (if (Utilities|Enum|Equal(Enum) (Variables|/Game/SpyroContent/Global_Assets/Global_Components/Base_AI_Character.Base_AI_Character_C|GetAICharacter_State (Variables|Default|GetWalking_AI_Character)) "NewEnumerator3")
          _
          (else
            (Default|ChangeAICharacterState (Variables|Default|GetWalking_AI_Character) "NewEnumerator2"))))
      (Attacking|AttackRadiusOverlapped))
    (else
      (goto _label))))

(event EventBeginPlay
  (|CallParentFunction)
  (Variables|Default|SetStarting_Yaw (.yaw (Transformation|GetActorRotation)))
  (EventDispatchers|BindEventtoHeatMetal (Variables|Default|GetDamageable) (delegate HeattheMetal))
  (EventDispatchers|BindEventtoMyStateChanged (Variables|Default|GetWalking_AI_Character) (delegate Custom|On%20Enemy%20State%20Changed))
  (bind _asspyro_persistant_data (Utilities|Casting|CastToSpyro_PersistantData (Game|GetGameInstance))
    (:then
      (EventDispatchers|BindEventtoDifficultyChanged _asspyro_persistant_data (delegate Custom|Set%20My%20Difficulty)))
    (:CastFailed
      _))
  (CallFunction|SetMyDifficulty)
  (Utilities|Time|SetTimerbyFunctionName 0 "fix frozen col bug" 0.5 true)
  (if (Variables|/Game/SpyroContent/Global_Assets/Global_Components/Base_AI_Character.Base_AI_Character_C|GetCan_Attack (Variables|Default|GetWalking_AI_Character))
    (Utilities|Time|SetTimerbyFunctionName 0 "Attack Radius Ping" 0.5 true)))

(event EventTick
  (params (DeltaSeconds :type Float%20%28single-precision%29))
  (|CallParentFunction DeltaSeconds)
  (CallFunction|LookatPlayer))

(fn ConstructionScript
  (|CallParentFunction))

(fn AttackRadiusOverlapped)

(fn SomethingOverlappedAttackRadius
  (params (Other%20Actor :type Object%20Object%20Reference) (Other%20Comp :type Object%20Object%20Reference))
  (bind _walking_ai_character (Variables|Default|GetWalking_AI_Character))
  (bind _aicharacter_state (Variables|/Game/SpyroContent/Global_Assets/Global_Components/Base_AI_Character.Base_AI_Character_C|GetAICharacter_State _walking_ai_character))
  (bind _asbp_base_playable (Utilities|Casting|CastToBP_Base_Playable Other%20Actor))
  (if (Math|Boolean|ANDBoolean (== (Variables|/Script/Engine.Character|GetCapsuleComponent _asbp_base_playable) Other%20Comp) (Variables|/Game/SpyroContent/Global_Assets/Global_Components/Base_AI_Character.Base_AI_Character_C|GetCan_Attack _walking_ai_character) (<= (Variables|Attacking|GetCurrent_Cooldown_Time) 0))
    (Utilities|Array|AddUnique (Variables|/Game/SpyroContent/Global_Assets/Global_Components/Base_AI_Character.Base_AI_Character_C|GetPlayers_I_Am_Alert_To (Variables|Default|GetWalking_AI_Character)) _asbp_base_playable)
    (if (and (or (Utilities|Enum|Equal(Enum) _aicharacter_state "NewEnumerator0") (Utilities|Enum|Equal(Enum) _aicharacter_state "NewEnumerator1")) (not (Utilities|Enum|Equal(Enum) (Variables|/Game/SpyroContent/Global_Assets/Global_Characters/Playable_Characters/BP_Base_Playable.BP_Base_Playable_C|GetPlayer_State _asbp_base_playable) "NewEnumerator11")))
      (CallFunction|AttackAfterDelay))))

(fn AttackRadiusPing
  (bind _attack_radius (Variables|Default|GetAttack_Radius))
  (bind _returnvalue (Transformation|GetWorldLocation _attack_radius))
  (if (Variables|Default|GetOff%20Camera%20Mercy)
    (bind _returnvalue_2 (CallFunction|AmIonCamera?))
    (if (and (not _returnvalue_2) (Utilities|Enum|Equal(Enum) (Variables|/Game/SpyroContent/Global_Assets/Global_Components/Base_AI_Character.Base_AI_Character_C|GetAICharacter_State (Variables|Default|GetWalking_AI_Character)) "NewEnumerator2"))
      (Default|ChangeAICharacterState (Variables|Default|GetWalking_AI_Character) "NewEnumerator1")))
  (bind _outhits (Collision|MultiSphereTraceForObjects _returnvalue _returnvalue (Variables|/Script/Engine.SphereComponent|GetSphereRadius _attack_radius) (Utilities|Array|MakeArray "ObjectTypeQuery3" "ObjectTypeQuery8" "ObjectTypeQuery9") false 0 "None"))
  (for _array_element _outhits
    (if (.bblockinghit _array_element)
      (Attacking|SomethingOverlappedAttackRadius (.hitactor _array_element) (.hitcomponent _array_element)))))

(fn LookatPlayer
  (bind _returnvalue (Utilities|Time|GetWorldDeltaSeconds))
  (bind _returnvalue_2 (Transformation|GetActorRotation))
  (bind _capsulecomponent (Variables|Default|GetCapsuleComponent))
  (bind _starting_yaw (Variables|Default|GetStarting_Yaw))
  (bind _walking_ai_character (Variables|Default|GetWalking_AI_Character))
  (bind _damageable (Variables|Default|GetDamageable))
  (bind _returnvalue_3 (Math|Rotator|MakeRotator 0.0 0.0 _starting_yaw))
  (bind _returnvalue_4 (Transformation|GetWorldRotation _capsulecomponent))
  (bind _returnvalue_5 (* _returnvalue 5.0))
  (bind (_roll _pitch) (Math|Rotator|BreakRotator _returnvalue_4))
  (Utilities|FlowControl|Sequence
    (:then_0
      (if (and (not (Variables|/Game/SpyroContent/Global_Assets/Global_Components/Damageable_Com.Damageable_Com_C|GetFrozen _damageable)) (not (Variables|/Game/SpyroContent/Global_Assets/Global_Components/Damageable_Com.Damageable_Com_C|GetParalyzed_by_Fear _damageable)))
        (if (|alertandattackconditions)
          (bind _closest_player1 (Default|GetNearestPlayerImAlertto (Variables|Default|GetWalking_AI_Character)))
          (Utilities|IsValid _closest_player1
            (:Is%20Valid
              (if (not (Math|Rotator|Equal(Rotator) (Transformation|GetWorldRotation (Variables|Default|GetCapsuleComponent)) (select (Variables|/Game/SpyroContent/Global_Assets/Global_Components/Base_AI_Character.Base_AI_Character_C|Gettilt%20to%20player (Variables|Default|GetWalking_AI_Character)) (Math|Rotator|MakeRotator (.roll (Math|Rotator|FindLookatRotation (Transformation|GetWorldLocation (Variables|Default|GetCapsuleComponent)) (Transformation|GetActorLocation _closest_player1))) (.pitch (Math|Rotator|FindLookatRotation (Transformation|GetWorldLocation (Variables|Default|GetCapsuleComponent)) (Transformation|GetActorLocation _closest_player1))) (.yaw (Math|Rotator|FindLookatRotation (Transformation|GetWorldLocation (Variables|Default|GetCapsuleComponent)) (Transformation|GetActorLocation _closest_player1)))) (Math|Rotator|MakeRotator _roll _pitch (.yaw (Math|Rotator|Lerp(Rotator) _returnvalue_4 (Math|Rotator|MakeRotator _roll _pitch (.yaw (Math|Rotator|FindLookatRotation (Transformation|GetWorldLocation (Variables|Default|GetCapsuleComponent)) (Transformation|GetActorLocation _closest_player1)))) _returnvalue_5 true)))) 0.1))
                (Transformation|SetWorldRotation (Variables|Default|GetCapsuleComponent) (select (Variables|/Game/SpyroContent/Global_Assets/Global_Components/Base_AI_Character.Base_AI_Character_C|Gettilt%20to%20player (Variables|Default|GetWalking_AI_Character)) (Math|Rotator|MakeRotator (.roll (Math|Rotator|FindLookatRotation (Transformation|GetWorldLocation (Variables|Default|GetCapsuleComponent)) (Transformation|GetActorLocation _closest_player1))) (.pitch (Math|Rotator|FindLookatRotation (Transformation|GetWorldLocation (Variables|Default|GetCapsuleComponent)) (Transformation|GetActorLocation _closest_player1))) (.yaw (Math|Rotator|FindLookatRotation (Transformation|GetWorldLocation (Variables|Default|GetCapsuleComponent)) (Transformation|GetActorLocation _closest_player1)))) (Math|Rotator|MakeRotator _roll _pitch (.yaw (Math|Rotator|Lerp(Rotator) _returnvalue_4 (Math|Rotator|MakeRotator _roll _pitch (.yaw (Math|Rotator|FindLookatRotation (Transformation|GetWorldLocation (Variables|Default|GetCapsuleComponent)) (Transformation|GetActorLocation _closest_player1)))) _returnvalue_5 true)))) false false))))
          (elif (Math|Boolean|ANDBoolean (not (Utilities|Enum|Equal(Enum) (Variables|/Game/SpyroContent/Global_Assets/Global_Components/Base_AI_Character.Base_AI_Character_C|GetAICharacter_State (Variables|Default|GetWalking_AI_Character)) "NewEnumerator3")) (or (Variables|/Game/SpyroContent/Global_Assets/Global_Components/Base_AI_Character.Base_AI_Character_C|GetCan_Become_Alert _walking_ai_character) (Math|Boolean|ANDBoolean (Variables|/Game/SpyroContent/Global_Assets/Global_Components/Base_AI_Character.Base_AI_Character_C|GetCan_Attack _walking_ai_character) (Utilities|Enum|Equal(Enum) (Variables|/Game/SpyroContent/Global_Assets/Global_Components/Base_AI_Character.Base_AI_Character_C|GetAttack_Behavior _walking_ai_character) "NewEnumerator0") (< (Utilities|Array|Length (Variables|/Game/SpyroContent/Global_Assets/Global_Components/Base_AI_Character.Base_AI_Character_C|GetPlayers_I_Am_Alert_To (Variables|Default|GetWalking_AI_Character))) 0))) (not (Math|Rotator|Equal(Rotator) _returnvalue_2 _returnvalue_3 0.1)) (not (Variables|/Game/SpyroContent/Global_Assets/Global_Components/Base_AI_Character.Base_AI_Character_C|GetNever%20Rotate,%20Has%20Flying%20AI (Variables|Default|GetWalking_AI_Character))))
            (Transformation|SetActorRotation (Math|Rotator|Lerp(Rotator) _returnvalue_2 _returnvalue_3 _returnvalue_5 true))))))
    (:then_1
      (return))))

(fn AttackCooldownCountdown
  (if (not (Utilities|Enum|Equal(Enum) (Variables|/Game/SpyroContent/Global_Assets/Global_Components/Base_AI_Character.Base_AI_Character_C|GetAICharacter_State (Variables|Default|GetWalking_AI_Character)) "NewEnumerator2"))
    (Variables|Attacking|SetCurrent_Cooldown_Time (select (< (- (Variables|Attacking|GetCurrent_Cooldown_Time) 1) 0) 0 (- (Variables|Attacking|GetCurrent_Cooldown_Time) 1)))))

(fn StartAttackCooldown
  (bind _min_antistunlock_cooldown (Variables|Attacking|GetMin_Antistunlock_Cooldown))
  (if (and (> (Variables|Attacking|GetMax_Attack_Cooldown) 0) (not (Utilities|Time|IsValidTimerHandle (Variables|Attacking|GetAttack%20Cooldown%20Timer))))
    (if (Utilities|Enum|Equal(Enum) (Variables|/Game/SpyroContent/Global_Assets/Global_Components/Base_AI_Character.Base_AI_Character_C|GetAICharacter_State (Variables|Default|GetWalking_AI_Character)) "NewEnumerator2")
      (Default|ChangeAICharacterState (Variables|Default|GetWalking_AI_Character) "NewEnumerator1"))
    (Variables|Attacking|SetCurrent_Cooldown_Time (select (and (< (Variables|Attacking|GetMax_Attack_Cooldown) _min_antistunlock_cooldown) (Variables|Difficulty|GetDamaged%20Player,%20Show%20Mercy)) _min_antistunlock_cooldown (Variables|Attacking|GetMax_Attack_Cooldown)))
    (bind _returnvalue (Utilities|Time|SetTimerbyFunctionName 0 "Attack Cooldown Countdown" 0.25 true))
    (Variables|Attacking|SetAttack%20Cooldown%20Timer _returnvalue)))

(fn IDamagedAPlayer
  (Variables|Difficulty|SetDamaged%20Player,%20Show%20Mercy true)
  (Utilities|Time|ClearandInvalidateTimerbyHandle (Variables|Attacking|GetAttack%20Cooldown%20Timer))
  (Attacking|StartAttackCooldown))

(fn FixFrozenColBug
  (if (Math|Boolean|ANDBoolean (Utilities|Enum|Equal(Enum) (Collision|GetCollisionObjectType (Variables|Default|GetCapsuleComponent)) "ECC_GameTraceChannel5") (> (Variables|Default|GetCustomTimeDilation) 0.0) (not (Utilities|Enum|Equal(Enum) (Variables|/Game/SpyroContent/Global_Assets/Global_Components/Base_AI_Character.Base_AI_Character_C|GetAICharacter_State (Variables|Default|GetWalking_AI_Character)) "NewEnumerator3")))
    (Collision|SetCollisionObjectType (Variables|Default|GetCapsuleComponent) "ECC_Pawn")
    (Development|PrintString (Utilities|String|Append (Utilities|GetObjectName self) ": I WAS IN FROZEN COL, BUT I WASNT FROZEN, SO I RETURNED TO PAWN STATE.") true true "(R=0.000000,G=0.660000,B=1.000000,A=1.000000)" 3e+01)))

(event Custom|Reset%20Heat%20Metal
  (bind _damageable (Variables|Default|GetDamageable))
  (bind _component_with_metal_material (Variables|/Game/SpyroContent/Global_Assets/Global_Components/Damageable_Com.Damageable_Com_C|GetComponent_with_Metal_Material _damageable))
  (Utilities|FlowControl|DoOnce false) ; enters at Reset
)

(event Custom|Heat%20Metal
  (bind _damageable (Variables|Default|GetDamageable))
  (bind _component_with_metal_material (Variables|/Game/SpyroContent/Global_Assets/Global_Components/Damageable_Com.Damageable_Com_C|GetComponent_with_Metal_Material _damageable))
  (bind _component_with_metal_material_2 (Variables|/Game/SpyroContent/Global_Assets/Global_Components/Damageable_Com.Damageable_Com_C|GetComponent_with_Metal_Material (Variables|Default|GetDamageable))
    (:then
      (Utilities|FlowControl|DoOnce false
        (:Completed
          (Utilities|Array|Clear (Variables|Default|GetDyn_Mat_Refs))
          (for (_ _array_index) (Rendering|Material|GetMaterials _component_with_metal_material_2)
            (if (>= (Utilities|Array|FindItem (Variables|/Game/SpyroContent/Global_Assets/Global_Components/Damageable_Com.Damageable_Com_C|GetMetal%20Material%20Indexes (Variables|Default|GetDamageable)) _array_index) 0)
              (bind _returnvalue (Rendering|Material|CreateDynamicMaterialInstance _component_with_metal_material _array_index (Rendering|Material|GetMaterial _component_with_metal_material _array_index) "None" :!class /Script/Engine.PrimitiveComponent))
              (Utilities|Array|Add (Variables|Default|GetDyn_Mat_Refs) _returnvalue)))
          (Utilities|FlowControl|Sequence
            (:then_0
              (bind _newtrack_0 (Timeline|Timeline_0 PlayFromStart)
                (:Update
                  (for _array_element (Variables|Default|GetDyn_Mat_Refs)
                    (Rendering|Material|SetVectorParameterValue _array_element "ColorChange" (Utilities|Struct|MakeLinearColor (.x _newtrack_0) (.y _newtrack_0) (.z _newtrack_0) 0.0) :!class /Script/Engine.MaterialInstanceDynamic)))))
            (:then_1
              (Utilities|FlowControl|Delay 1.0)
              (CallFunction|ResetHeatMetal))))))
    (:else)))