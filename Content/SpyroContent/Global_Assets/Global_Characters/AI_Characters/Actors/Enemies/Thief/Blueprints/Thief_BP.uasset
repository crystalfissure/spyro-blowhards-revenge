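; Thief enemy Blueprint that can carry a stolen collectable attached to its mesh and reports the theft and its death to that item's NPC_Award_Item component.
; State changes drive idle countdowns, a cooldown-locked laugh while attacking, and death, which credits the killing player before detaching the item.
; The S1 treasure save setting selects the death scream and mutes laughs.
; A looping timer toggles supercharge dust at high speed.
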(event Custom|On%20Thief%20State%20Change
  (bind _walking_ai_character (Variables|Default|GetWalking_AI_Character))
  (Utilities|FlowControl|Sequence
    (:then_0
      (switch Utilities|FlowControl|Switch|SwitchonAICharacter_States (Variables|/Game/SpyroContent/Global_Assets/Global_Components/Base_AI_Character.Base_AI_Character_C|GetAICharacter_State (Variables|Default|GetWalking_AI_Character))
        (:NewEnumerator1
          (Default|StartIdleCountdownTimer _walking_ai_character)
          (Variables|/Game/SpyroContent/Global_Assets/Global_Components/Base_AI_Character.Base_AI_Character_C|SetIdle_Animation_Countdown (Variables|Default|GetWalking_AI_Character) 0))
        (:NewEnumerator2
          (CallFunction|LaughandRunAway))
        (:NewEnumerator3
          (|ThiefDeathProcess))))
    (:then_1
      (if (not (Utilities|Enum|Equal(Enum) (Variables|/Game/SpyroContent/Global_Assets/Global_Components/Base_AI_Character.Base_AI_Character_C|GetAICharacter_State _walking_ai_character) "NewEnumerator1"))
        (Default|StopIdleCountdownTimer _walking_ai_character)))))

(event Custom|Remove%20Laugh%20Lock
  (Utilities|FlowControl|Delay 1.0)
  (Variables|Default|SetLaugh%20Lock false))

(event Custom|Delayed%20Self-Destruct
  (Utilities|FlowControl|Delay 3.0)
  (bind _stolen_collectable (Variables|Default|GetStolen_Collectable)
    (:then
      (Transformation|DetachFromActor _stolen_collectable "KeepWorld" "KeepWorld" "KeepWorld"))
    (:else
      _))
  (Actor|DestroyActor))

(event EventBeginPlay
  (bind _stolen_collectable (Variables|Default|GetStolen_Collectable))
  (bind _drops_items (Variables|Default|GetDrops_Items))
  (bind _items_to_drop (Variables|/Game/SpyroContent/Global_Assets/Global_Components/Drops_Items.Drops_Items_C|GetItems_to_Drop _drops_items))
  (|CallParentFunction)
  (Utilities|Time|SetTimerbyFunctionName 0 "supercharge dust check" 0.2 true)
  (Variables|/Game/SpyroContent/Global_Assets/Global_Components/Damageable_Com.Damageable_Com_C|SetObject's%20Hitbox%20Component (Variables|Default|GetDamageable) (Variables|Default|GetHitbox))
  (EventDispatchers|BindEventtoMyStateChanged (Variables|Default|GetWalking_AI_Character) (delegate Custom|On%20Thief%20State%20Change))
  (CallFunction|OnThiefStateChange)
  (bind _asspyro_persistant_data (Utilities|Casting|CastToSpyro_PersistantData (Game|GetGameInstance)))
  (EventDispatchers|BindEventtoChangeTreasureSkins _asspyro_persistant_data (delegate S1DeathScream))
  (Utilities|FlowControl|Delay 0.2)
  (CallFunction|SetDeathScream)
  (bind _stolen_collectable_2 (Variables|Default|GetStolen_Collectable)
    (:then
      (Utilities|Array|Clear _items_to_drop)
      (Utilities|Array|SetArrayElem _items_to_drop 0 "/Game/SpyroContent/Global_Assets/Global_Level_Items/Treasure_Containers/Dummy_Item_BP.Dummy_Item_BP_C" true)
      ;[0.207 0.03193 0.5573 1 14] qtderg experimental modification
      ;
      ; By plugging Is Not Valid to Set Actor Rotation, thieves can now steal things other than collectables. Use with caution
      (Utilities|IsValid (Actor|GetComponentbyClass _stolen_collectable_2 "/Game/SpyroContent/Global_Assets/Global_Components/NPC_Award_Item.NPC_Award_Item_C")
        (:Is%20Valid
          (Default|CallAThiefStoleMe (Actor|GetComponentbyClass _stolen_collectable_2 "/Game/SpyroContent/Global_Assets/Global_Components/NPC_Award_Item.NPC_Award_Item_C")))
        (:Is%20Not%20Valid
          _))
      (Transformation|SetActorRotation _stolen_collectable (Math|Rotator|MakeRotator 0.0 0.0 (.yaw (Transformation|GetActorRotation))))
      (Utilities|FlowControl|Delay 0.2)
      (Transformation|AttachComponentToComponent _stolen_collectable (Variables|Character|GetMesh) "Item_Attach" "SnapToTarget" "KeepWorld" "KeepWorld" false))
    (:else
      (if (Variables|Default|GetHas%20a%20Stolen%20Collectible)
        (Actor|DestroyActor)))))

(event EventRunningDirectionChanged
  (|CallParentFunction)
  (if (Utilities|Enum|Equal(Enum) (Variables|/Game/SpyroContent/Global_Assets/Global_Components/Base_AI_Character.Base_AI_Character_C|GetAICharacter_State (Variables|Default|GetWalking_AI_Character)) "NewEnumerator2")
    (Utilities|FlowControl|Delay 0.2)
    (CallFunction|LaughandRunAway)))

(fn ConstructionScript
  (|CallParentFunction))

(fn LaughandRunAway
  (bind _damageable (Variables|Default|GetDamageable))
  (bind _character_s_voice (Variables|Default|GetCharacter's%20Voice))
  (if (Math|Boolean|ANDBoolean (not (Variables|Default|GetS1_Mode)) (not (Variables|Default|GetLaugh%20Lock)) (not (Utilities|Enum|Equal(Enum) (Variables|/Game/SpyroContent/Global_Assets/Global_Components/Base_AI_Character.Base_AI_Character_C|GetAICharacter_State (Variables|Default|GetWalking_AI_Character)) "NewEnumerator3")) (not (Variables|/Game/SpyroContent/Global_Assets/Global_Components/Damageable_Com.Damageable_Com_C|GetFrozen _damageable)) (not (Variables|/Game/SpyroContent/Global_Assets/Global_Components/Damageable_Com.Damageable_Com_C|GetParalyzed_by_Fear _damageable)))
    (Audio|Components|Audio|SetSound _character_s_voice "/Game/SpyroContent/Global_Assets/Global_Characters/AI_Characters/Actors/Enemies/Thief/Audio/ThiefLulz1.ThiefLulz1")
    (Audio|Components|Audio|Play _character_s_voice 0.0)
    (Variables|Default|SetLaugh%20Lock true)
    (CallFunction|RemoveLaughLock)))

(fn SuperchargeDustCheck
  (if (and (> (Math|Vector|VectorLength (Transformation|GetVelocity)) 1.65e+03) (not (Utilities|Enum|Equal(Enum) (Variables|/Game/SpyroContent/Global_Assets/Global_Components/Base_AI_Character.Base_AI_Character_C|GetAICharacter_State (Variables|Default|GetWalking_AI_Character)) "NewEnumerator3")))
    (if (not (Components|Activation|IsActive (Variables|Default|Getsupercharge_dust)))
      (Components|Activation|Activate (Variables|Default|Getsupercharge_dust) false))
    (elif (Components|Activation|IsActive (Variables|Default|Getsupercharge_dust))
      (Components|Activation|Deactivate (Variables|Default|Getsupercharge_dust)))))

(event Custom|Set%20Death%20Scream
  (bind _asspyro_save_data (CallFunction|LoadSpyroGame self))
  (Utilities|IsValid _asspyro_save_data
    (:Is%20Valid
      (Variables|Default|SetS1_Mode (Variables|/Game/SpyroContent/Global_Assets/Global_SaveData/Spyro_SaveData.Spyro_SaveData_C|GetS1_Treasure _asspyro_save_data))
      (Variables|/Game/SpyroContent/Global_Assets/Global_Components/Base_AI_Character.Base_AI_Character_C|SetDeath_Scream (Variables|Default|GetWalking_AI_Character) (select (Variables|/Game/SpyroContent/Global_Assets/Global_SaveData/Spyro_SaveData.Spyro_SaveData_C|GetS1_Treasure _asspyro_save_data) "/Game/SpyroContent/Global_Assets/Global_Characters/AI_Characters/Actors/Enemies/Thief/Audio/EggThiefHit1.EggThiefHit1" "/Game/SpyroContent/Global_Assets/Global_Characters/AI_Characters/Actors/Enemies/Thief/Audio/ThiefHit1.ThiefHit1")))))