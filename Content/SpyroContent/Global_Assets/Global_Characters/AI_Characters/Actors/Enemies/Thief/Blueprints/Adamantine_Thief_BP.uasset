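; Adamantine_Thief_BP is a child Blueprint of an AI thief enemy that adjusts how it responds to damage.
; On BeginPlay it binds a handler to its Damageable component's deal-damage event.
; The handler confirms damage as successfully dealt only for one specific damage type flagged as super damage, and only while the AI character is outside one particular state.
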(event Custom|On%20Damage%20Dealt
  (bind _damageable (Variables|Default|GetDamageable))
  (if (Math|Boolean|ANDBoolean (not (Utilities|Enum|Equal(Enum) (Variables|/Game/SpyroContent/Global_Assets/Global_Components/Base_AI_Character.Base_AI_Character_C|GetAICharacter_State (Variables|Default|GetWalking_AI_Character)) "NewEnumerator3")) (Utilities|Enum|Equal(Enum) (Variables|/Game/SpyroContent/Global_Assets/Global_Components/Damageable_Com.Damageable_Com_C|GetDeal%20Damage%20-%20Damage%20Type _damageable) "NewEnumerator4") (Variables|/Game/SpyroContent/Global_Assets/Global_Components/Damageable_Com.Damageable_Com_C|GetDeal%20Damage%20-%20Super%20Damage _damageable))
    (Default|CallDamageWasSuccessfullyDealt (Variables|Default|GetDamageable))))

(event EventBeginPlay
  (|CallParentFunction)
  (EventDispatchers|BindEventtoCallDealDamage (Variables|Default|GetDamageable) (delegate Custom|On%20Damage%20Dealt)))

(fn ConstructionScript
  (|CallParentFunction))