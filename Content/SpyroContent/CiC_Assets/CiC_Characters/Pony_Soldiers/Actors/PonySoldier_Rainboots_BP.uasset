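; Rainboots Pony Soldier enemy that idles by splashing a linked umbrella pony (IdleTauntTarget), keeping both Anim Blueprints in sync.
; Alert, attack or death stops the splashing and its level sequence, and damage to the target can alert it.
; Freeze-type damage pauses the sequence until it thaws or stops being afraid, and finishing it changes idle pose and yaw.
; Item-dropper resets restore the splashing unless either pony is permanently dead.
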(event Custom|On%20Pony%20State%20Changed
  (switch Utilities|FlowControl|Switch|SwitchonAICharacter_States (Variables|/Game/SpyroContent/Global_Assets/Global_Components/Base_AI_Character.Base_AI_Character_C|GetAICharacter_State (Variables|Default|GetWalking_AI_Character))
    (:NewEnumerator1
      _)
    (:NewEnumerator2
      _)
    (:NewEnumerator3
      (Variables|/Game/SpyroContent/Global_Assets/Global_Components/Base_AI_Character.Base_AI_Character_C|SetCan_Become_Alert (Variables|Default|GetWalking_AI_Character) true)))
  (bind _aspony_soldier_rainboots_abp (Utilities|Casting|CastToPonySoldier_Rainboots_ABP (Components|SkeletalMesh|GetAnimInstance (Variables|Character|GetMesh)))
    (:then
      (Variables|/Game/SpyroContent/CiC_Assets/CiC_Characters/Pony_Soldiers/ABPs/PonySoldier_Rainboots_ABP.PonySoldier_Rainboots_ABP_C|SetABP_RainbootsPony_State _aspony_soldier_rainboots_abp "NewEnumerator0"))
    (:CastFailed
      _))
  (bind _idle_taunt_target (Variables|Default|GetIdle%20Taunt%20Target)
    (:then
      (bind _aspony_soldier_umbrella_abp (Utilities|Casting|CastToPonySoldier_Umbrella_ABP (Components|SkeletalMesh|GetAnimInstance (Variables|/Script/Engine.Character|GetMesh _idle_taunt_target)))
        (:then
          (Variables|/Game/SpyroContent/CiC_Assets/CiC_Characters/Pony_Soldiers/ABPs/PonySoldier_Umbrella_ABP.PonySoldier_Umbrella_ABP_C|SetisGettingSplashed _aspony_soldier_umbrella_abp false))
        (:CastFailed
          _)))
    (:else
      _))
  (bind _my_sequence (Variables|Default|GetMy%20Sequence)
    (:then
      (Sequencer|Player|Stop (Variables|/Script/LevelSequence.LevelSequenceActor|GetSequencePlayer _my_sequence) :!class /Script/MovieScene.MovieSceneSequencePlayer))
    (:else)))

(event Custom|On%20Pony%20Reset
  (|PonyResetEvent))

(event Custom|On%20Sequence%20Finished
  (if (Utilities|Enum|Equal(Enum) (Variables|/Game/SpyroContent/Global_Assets/Global_Components/Base_AI_Character.Base_AI_Character_C|GetAICharacter_State (Variables|Default|GetWalking_AI_Character)) "NewEnumerator0")
    (bind _aspony_soldier_rainboots_abp (Utilities|Casting|CastToPonySoldier_Rainboots_ABP (Components|SkeletalMesh|GetAnimInstance (Variables|Character|GetMesh)))
      (:then
        (Variables|/Game/SpyroContent/CiC_Assets/CiC_Characters/Pony_Soldiers/ABPs/PonySoldier_Rainboots_ABP.PonySoldier_Rainboots_ABP_C|SetABP_RainbootsPony_State _aspony_soldier_rainboots_abp "NewEnumerator3"))
      (:CastFailed
        _))
    (Transformation|SetActorRotation (Math|Rotator|MakeRotator 0.0 0.0 (Variables|Default|GetSequence%20Finished%20Yaw)))))

(event Custom|On%20Big%20Pony%20Killed
  (bind _aspony_soldier_rainboots_abp (Utilities|Casting|CastToPonySoldier_Rainboots_ABP (Components|SkeletalMesh|GetAnimInstance (Variables|Character|GetMesh))))
  (if (Utilities|Enum|Equal(Enum) (Variables|/Game/SpyroContent/CiC_Assets/CiC_Characters/Pony_Soldiers/ABPs/PonySoldier_Rainboots_ABP.PonySoldier_Rainboots_ABP_C|GetABP_RainbootsPony_State _aspony_soldier_rainboots_abp) "NewEnumerator1")
    (Default|ChangeAICharacterState (Variables|Default|GetWalking_AI_Character) "NewEnumerator1")))

(event Custom|On%20Frozen
  (bind _damageable (Variables|Default|GetDamageable))
  (bind _deal_damage___damage_type (Variables|/Game/SpyroContent/Global_Assets/Global_Components/Damageable_Com.Damageable_Com_C|GetDeal%20Damage%20-%20Damage%20Type _damageable))
  (if (or (Utilities|Enum|Equal(Enum) _deal_damage___damage_type "NewEnumerator7") (Utilities|Enum|Equal(Enum) _deal_damage___damage_type "NewEnumerator8"))
    (Class|MovieSceneSequencePlayer|StopatCurrentTime (Variables|/Script/LevelSequence.LevelSequenceActor|GetSequencePlayer (Variables|Default|GetMy%20Sequence)))))

(event Custom|Resume%20Running%20After%20Unfrozen
  (bind _aspony_soldier_rainboots_abp (Utilities|Casting|CastToPonySoldier_Rainboots_ABP (Components|SkeletalMesh|GetAnimInstance (Variables|Character|GetMesh))))
  (if (and (Utilities|Enum|Equal(Enum) (Variables|/Game/SpyroContent/CiC_Assets/CiC_Characters/Pony_Soldiers/ABPs/PonySoldier_Rainboots_ABP.PonySoldier_Rainboots_ABP_C|GetABP_RainbootsPony_State _aspony_soldier_rainboots_abp) "NewEnumerator2") (Utilities|Enum|Equal(Enum) (Variables|/Game/SpyroContent/Global_Assets/Global_Components/Base_AI_Character.Base_AI_Character_C|GetAICharacter_State (Variables|Default|GetWalking_AI_Character)) "NewEnumerator0"))
    (Sequencer|Player|Play (Variables|/Script/LevelSequence.LevelSequenceActor|GetSequencePlayer (Variables|Default|GetMy%20Sequence)) :!class /Script/MovieScene.MovieSceneSequencePlayer)))

(event EventBeginPlay
  (bind _damageable (Variables|Default|GetDamageable))
  (|CallParentFunction)
  (EventDispatchers|BindEventtoItemDropperSuccessfullyReset (Variables|Default|GetDrops_Items) (delegate Custom|On%20Pony%20Reset))
  (EventDispatchers|BindEventtoMyStateChanged (Variables|Default|GetWalking_AI_Character) (delegate Custom|On%20Pony%20State%20Changed))
  (Variables|Default|GetIdle%20Taunt%20Target
    (:then
      (bind _aspony_soldier_rainboots_abp (Utilities|Casting|CastToPonySoldier_Rainboots_ABP (Components|SkeletalMesh|GetAnimInstance (Variables|Character|GetMesh)))
        (:then
          (Variables|/Game/SpyroContent/CiC_Assets/CiC_Characters/Pony_Soldiers/ABPs/PonySoldier_Rainboots_ABP.PonySoldier_Rainboots_ABP_C|SetABP_RainbootsPony_State _aspony_soldier_rainboots_abp "NewEnumerator1"))
        (:CastFailed
          _))
      (bind _aspony_soldier_umbrella_abp (Utilities|Casting|CastToPonySoldier_Umbrella_ABP (Components|SkeletalMesh|GetAnimInstance (Variables|/Script/Engine.Character|GetMesh (Variables|Default|GetIdle%20Taunt%20Target))))
        (:then
          (Variables|/Game/SpyroContent/CiC_Assets/CiC_Characters/Pony_Soldiers/ABPs/PonySoldier_Umbrella_ABP.PonySoldier_Umbrella_ABP_C|SetisGettingSplashed _aspony_soldier_umbrella_abp true))
        (:CastFailed
          _)))
    (:else
      _))
  (EventDispatchers|BindEventtoOnFinished (Variables|/Script/LevelSequence.LevelSequenceActor|GetSequencePlayer (Variables|Default|GetMy%20Sequence)) (delegate Custom|On%20Sequence%20Finished))
  (bind _idle_taunt_target (Variables|Default|GetIdle%20Taunt%20Target)
    (:then
      (EventDispatchers|BindEventtoDamageWasSuccessfullyDealt (Variables|/Game/SpyroContent/Global_Assets/Global_Characters/AI_Characters/Actors/Base_AICharacter_BP.Base_AICharacter_BP_C|GetDamageable _idle_taunt_target) (delegate Custom|On%20Big%20Pony%20Killed)))
    (:else
      _))
  (EventDispatchers|BindEventtoDamageWasSuccessfullyDealt (Variables|Default|GetDamageable) (delegate Custom|On%20Frozen))
  (EventDispatchers|BindEventtoMeltedfromIce _damageable (delegate Custom|Resume%20Running%20After%20Unfrozen))
  (EventDispatchers|BindEventtoCallStopBeingAfraid _damageable (delegate Custom|Resume%20Running%20After%20Unfrozen)))

(fn ConstructionScript
  (|CallParentFunction))