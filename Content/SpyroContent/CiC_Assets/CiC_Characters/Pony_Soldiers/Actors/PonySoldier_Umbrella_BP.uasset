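; Umbrella-wielding Pony Soldier enemy that extends a parent walking-AI character and spits a horse sound when it goes from Idle to Alert.
; While attacking, unless frozen or fear-paralyzed, its umbrella hitbox damages damageable actors, sparing players in one specific state.
; Players in that same state damage the pony through its Headbash hitbox.
; Difficulty, derived from saved skill level when Dynamic, tunes attack cooldown, radius and delay.
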(event OnComponentBeginOverlap(Umbrella_Hitbox)
  (params (OverlappedComponent :type Primitive%20Component%20Object%20Reference) (OtherActor :type Actor%20Object%20Reference) (OtherComp :type Primitive%20Component%20Object%20Reference) (OtherBodyIndex :type Integer) (bFromSweep :type Boolean) (SweepResult :type Hit%20Result%20Structure%20%28by%20ref%29))
  (bind _returnvalue (Actor|GetComponentbyClass OtherActor "/Game/SpyroContent/Global_Assets/Global_Components/Damageable_Com.Damageable_Com_C"))
  (bind _damageable (Variables|Default|GetDamageable))
  (if (Math|Boolean|ANDBoolean (== (Variables|/Game/SpyroContent/Global_Assets/Global_Components/Damageable_Com.Damageable_Com_C|GetObject's%20Hitbox%20Component _returnvalue) OtherComp) (not (== self OtherActor)) (Utilities|Enum|Equal(Enum) (Variables|/Game/SpyroContent/Global_Assets/Global_Components/Base_AI_Character.Base_AI_Character_C|GetAICharacter_State (Variables|Default|GetWalking_AI_Character)) "NewEnumerator2") (not (Variables|/Game/SpyroContent/Global_Assets/Global_Components/Damageable_Com.Damageable_Com_C|GetFrozen _damageable)) (not (Variables|/Game/SpyroContent/Global_Assets/Global_Components/Damageable_Com.Damageable_Com_C|GetParalyzed_by_Fear _damageable)))
    (bind _asbp_base_playable (Utilities|Casting|CastToBP_Base_Playable OtherActor)
      (:then
        (if (not (Utilities|Enum|Equal(Enum) (Variables|/Game/SpyroContent/Global_Assets/Global_Characters/Playable_Characters/BP_Base_Playable.BP_Base_Playable_C|GetPlayer_State _asbp_base_playable) "NewEnumerator8"))
          (Default|DealDamage _returnvalue "NewEnumerator2" "0, 0, 0" true self false :!label _label)))
      (:CastFailed
        (goto _label)))))

(event OnComponentBeginOverlap(Headbash_Hitbox)
  (params (OverlappedComponent :type Primitive%20Component%20Object%20Reference) (OtherActor :type Actor%20Object%20Reference) (OtherComp :type Primitive%20Component%20Object%20Reference) (OtherBodyIndex :type Integer) (bFromSweep :type Boolean) (SweepResult :type Hit%20Result%20Structure%20%28by%20ref%29))
  (bind _asbp_base_playable (Utilities|Casting|CastToBP_Base_Playable OtherActor))
  (if (and (Utilities|Enum|Equal(Enum) (Variables|/Game/SpyroContent/Global_Assets/Global_Characters/Playable_Characters/BP_Base_Playable.BP_Base_Playable_C|GetPlayer_State _asbp_base_playable) "NewEnumerator8") (== (Variables|/Script/Engine.Character|GetCapsuleComponent _asbp_base_playable) OtherComp))
    (Default|DealDamage (Variables|Default|GetDamageable) "NewEnumerator2" "0, 0, 0" true _asbp_base_playable false)))

(event Custom|On%20Pony%20State%20Changed
  (bind _character_s_voice (Variables|Default|GetCharacter's%20Voice))
  (switch Utilities|FlowControl|Switch|SwitchonAICharacter_States (Variables|/Game/SpyroContent/Global_Assets/Global_Components/Base_AI_Character.Base_AI_Character_C|GetAICharacter_State (Variables|Default|GetWalking_AI_Character))
    (:NewEnumerator1
      (if (Utilities|Enum|Equal(Enum) (Variables|/Game/SpyroContent/Global_Assets/Global_Components/Base_AI_Character.Base_AI_Character_C|GetPrevious%20AI%20State (Variables|Default|GetWalking_AI_Character)) "NewEnumerator0")
        (Audio|Components|Audio|SetSound _character_s_voice "/Game/SpyroContent/CiC_Assets/CiC_Characters/Pony_Soldiers/Audio/horse_spit.horse_spit")
        (Audio|Components|Audio|Play _character_s_voice 0.0)))))

(event EventSetMyDifficulty
  (bind _returnvalue (Math|Float|MakeLiteralFloat 4.8e+02))
  (|CallParentFunction)
  (bind _asspyro_universal_save_data (CallFunction|LoadUniversalSave))
  (if (Utilities|Enum|Equal(Enum) (Variables|/Game/SpyroContent/Global_Assets/Global_SaveData/Spyro_Universal_Save_Data.Spyro_Universal_Save_Data_C|GetDifficulty _asspyro_universal_save_data) "NewEnumerator4")
    (bind _asspyro_save_data (CallFunction|LoadSpyroGame self))
    (bind _difficulty (CallFunction|ConvertSkillLevelFloattoEnum (Variables|/Game/SpyroContent/Global_Assets/Global_SaveData/Spyro_SaveData.Spyro_SaveData_C|GetSkill_Level _asspyro_save_data)))
    (Variables|Default|SetMax_Attack_Cooldown (Utilities|Select :Index _difficulty :NewEnumerator4 9 :NewEnumerator0 16 :NewEnumerator1 9 :NewEnumerator2 3 :NewEnumerator3 1))
    (Components|Sphere|SetSphereRadius (Variables|Default|GetAttack_Radius) (Utilities|Select :Index _difficulty :NewEnumerator4 788.0 :NewEnumerator0 788.0 :NewEnumerator1 768.0 :NewEnumerator2 _returnvalue :NewEnumerator3 _returnvalue) true)
    (Variables|Default|SetAttack%20Delay (Utilities|Select :Index _difficulty :NewEnumerator4 0.5 :NewEnumerator0 1.0 :NewEnumerator1 0.5 :NewEnumerator2 0.0 :NewEnumerator3 0.0))
    (else
      (Variables|Default|SetMax_Attack_Cooldown (Utilities|Select :Index (Variables|/Game/SpyroContent/Global_Assets/Global_SaveData/Spyro_Universal_Save_Data.Spyro_Universal_Save_Data_C|GetDifficulty _asspyro_universal_save_data) :NewEnumerator4 9 :NewEnumerator0 16 :NewEnumerator1 9 :NewEnumerator2 3 :NewEnumerator3 1))
      (Components|Sphere|SetSphereRadius (Variables|Default|GetAttack_Radius) (Utilities|Select :Index (Variables|/Game/SpyroContent/Global_Assets/Global_SaveData/Spyro_Universal_Save_Data.Spyro_Universal_Save_Data_C|GetDifficulty _asspyro_universal_save_data) :NewEnumerator4 788.0 :NewEnumerator0 788.0 :NewEnumerator1 768.0 :NewEnumerator2 _returnvalue :NewEnumerator3 _returnvalue) true)
      (Variables|Default|SetAttack%20Delay (Utilities|Select :Index (Variables|/Game/SpyroContent/Global_Assets/Global_SaveData/Spyro_Universal_Save_Data.Spyro_Universal_Save_Data_C|GetDifficulty _asspyro_universal_save_data) :NewEnumerator4 0.5 :NewEnumerator0 1.0 :NewEnumerator1 0.5 :NewEnumerator2 0.0 :NewEnumerator3 0.0))))
  (if (> (Variables|Default|GetCurrent_Cooldown_Time) (Variables|Default|GetMax_Attack_Cooldown))
    (Variables|Default|SetCurrent_Cooldown_Time (Variables|Default|GetMax_Attack_Cooldown))))

(event EventBeginPlay
  (|CallParentFunction)
  (EventDispatchers|BindEventtoMyStateChanged (Variables|Default|GetWalking_AI_Character) (delegate Custom|On%20Pony%20State%20Changed)))

(fn ConstructionScript
  (|CallParentFunction))