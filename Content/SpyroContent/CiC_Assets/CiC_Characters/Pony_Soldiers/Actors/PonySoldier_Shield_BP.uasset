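; Shield-bearing Pony Soldier enemy, a walking AI character with a sword attack, built on a parent soldier class.
; AI state changes raise the shield hitbox while Alert and drop it otherwise; sword overlaps deal damage only while Attacking.
; Attack cooldown and delay follow difficulty, using saved player skill level on Dynamic.
; An optional MyEnemy is faced when idle, with a looping timer telling the AnimBP whether it is dead or out of range.
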(event OnComponentBeginOverlap(Sword_Hitbox)
  (params (OverlappedComponent :type Primitive%20Component%20Object%20Reference) (OtherActor :type Actor%20Object%20Reference) (OtherComp :type Primitive%20Component%20Object%20Reference) (OtherBodyIndex :type Integer) (bFromSweep :type Boolean) (SweepResult :type Hit%20Result%20Structure%20%28by%20ref%29))
  (bind _returnvalue (Actor|GetComponentbyClass OtherActor "/Game/SpyroContent/Global_Assets/Global_Components/Damageable_Com.Damageable_Com_C"))
  (bind _damageable (Variables|Default|GetDamageable))
  (if (Math|Boolean|ANDBoolean (== (Variables|/Game/SpyroContent/Global_Assets/Global_Components/Damageable_Com.Damageable_Com_C|GetObject's%20Hitbox%20Component _returnvalue) OtherComp) (not (== self OtherActor)) (Utilities|Enum|Equal(Enum) (Variables|/Game/SpyroContent/Global_Assets/Global_Components/Base_AI_Character.Base_AI_Character_C|GetAICharacter_State (Variables|Default|GetWalking_AI_Character)) "NewEnumerator2") (not (Variables|/Game/SpyroContent/Global_Assets/Global_Components/Damageable_Com.Damageable_Com_C|GetFrozen _damageable)) (not (Variables|/Game/SpyroContent/Global_Assets/Global_Components/Damageable_Com.Damageable_Com_C|GetParalyzed_by_Fear _damageable)))
    (bind _asbp_base_playable (Utilities|Casting|CastToBP_Base_Playable OtherActor)
      (:then
        (if (not (Utilities|Enum|Equal(Enum) (Variables|/Game/SpyroContent/Global_Assets/Global_Characters/Playable_Characters/BP_Base_Playable.BP_Base_Playable_C|GetPlayer_State _asbp_base_playable) "NewEnumerator8"))
          (Default|DealDamage _returnvalue "NewEnumerator0" "0, 0, 0" false self false :!label _label)))
      (:CastFailed
        (goto _label)))))

(event Custom|On%20Pony%20State%20Changed
  (bind _character_s_voice (Variables|Default|GetCharacter's%20Voice))
  (switch Utilities|FlowControl|Switch|SwitchonAICharacter_States (Variables|/Game/SpyroContent/Global_Assets/Global_Components/Base_AI_Character.Base_AI_Character_C|GetAICharacter_State (Variables|Default|GetWalking_AI_Character))
    (:NewEnumerator0
      (Collision|SetCollisionEnabled (Variables|Default|GetShield_Hitbox) "NoCollision" :!label _label))
    (:NewEnumerator1
      (Collision|SetCollisionEnabled (Variables|Default|GetShield_Hitbox) "QueryAndPhysics")
      (if (Utilities|Enum|Equal(Enum) (Variables|/Game/SpyroContent/Global_Assets/Global_Components/Base_AI_Character.Base_AI_Character_C|GetPrevious%20AI%20State (Variables|Default|GetWalking_AI_Character)) "NewEnumerator0")
        (Audio|Components|Audio|SetSound _character_s_voice "/Game/SpyroContent/CiC_Assets/CiC_Characters/Pony_Soldiers/Audio/horse_spit.horse_spit")
        (Audio|Components|Audio|Play _character_s_voice 0.0)))
    (:NewEnumerator2
      (goto _label))
    (:NewEnumerator3
      (goto _label))))

(event EventSetMyDifficulty
  (|CallParentFunction)
  (bind _asspyro_universal_save_data (CallFunction|LoadUniversalSave))
  (if (Utilities|Enum|Equal(Enum) (Variables|/Game/SpyroContent/Global_Assets/Global_SaveData/Spyro_Universal_Save_Data.Spyro_Universal_Save_Data_C|GetDifficulty _asspyro_universal_save_data) "NewEnumerator4")
    (bind _asspyro_save_data (CallFunction|LoadSpyroGame self))
    (bind _difficulty (CallFunction|ConvertSkillLevelFloattoEnum (Variables|/Game/SpyroContent/Global_Assets/Global_SaveData/Spyro_SaveData.Spyro_SaveData_C|GetSkill_Level _asspyro_save_data)))
    (Variables|Default|SetMax_Attack_Cooldown (Utilities|Select :Index _difficulty :NewEnumerator4 9 :NewEnumerator0 16 :NewEnumerator1 9 :NewEnumerator2 3 :NewEnumerator3 1))
    (Variables|Default|SetAttack%20Delay (Utilities|Select :Index _difficulty :NewEnumerator4 0.5 :NewEnumerator0 1.0 :NewEnumerator1 0.5 :NewEnumerator2 0.0 :NewEnumerator3 0.0))
    (else
      (Variables|Default|SetMax_Attack_Cooldown (Utilities|Select :Index (Variables|/Game/SpyroContent/Global_Assets/Global_SaveData/Spyro_Universal_Save_Data.Spyro_Universal_Save_Data_C|GetDifficulty _asspyro_universal_save_data) :NewEnumerator4 9 :NewEnumerator0 16 :NewEnumerator1 9 :NewEnumerator2 3 :NewEnumerator3 1))
      (Variables|Default|SetAttack%20Delay (Utilities|Select :Index (Variables|/Game/SpyroContent/Global_Assets/Global_SaveData/Spyro_Universal_Save_Data.Spyro_Universal_Save_Data_C|GetDifficulty _asspyro_universal_save_data) :NewEnumerator4 0.5 :NewEnumerator0 1.0 :NewEnumerator1 0.5 :NewEnumerator2 0.0 :NewEnumerator3 0.0))))
  (if (> (Variables|Default|GetCurrent_Cooldown_Time) (Variables|Default|GetMax_Attack_Cooldown))
    (Variables|Default|SetCurrent_Cooldown_Time (Variables|Default|GetMax_Attack_Cooldown))))

(event EventBeginPlay
  (bind _damageable (Variables|Default|GetDamageable))
  (|CallParentFunction)
  (EventDispatchers|BindEventtoMyStateChanged (Variables|Default|GetWalking_AI_Character) (delegate Custom|On%20Pony%20State%20Changed))
  (Variables|/Game/SpyroContent/Global_Assets/Global_Components/Damageable_Com.Damageable_Com_C|SetObject's%20Shield%20Component _damageable (Variables|Default|GetShield_Hitbox))
  (Variables|/Game/SpyroContent/Global_Assets/Global_Components/Damageable_Com.Damageable_Com_C|SetComponent_with_Metal_Material _damageable (Variables|Character|GetMesh))
  (Utilities|FlowControl|Delay (Variables|Default|Getanim%20delay))
  (bind _aspony_soldier_shield_abp (Utilities|Casting|CastToPonySoldier_Shield_ABP (Components|SkeletalMesh|GetAnimInstance (Variables|Character|GetMesh))))
  (Variables|/Game/SpyroContent/CiC_Assets/CiC_Characters/Pony_Soldiers/ABPs/PonySoldier_Shield_ABP.PonySoldier_Shield_ABP_C|Setunder%20attack _aspony_soldier_shield_abp (not (Variables|Default|Getchilling)))
  (Variables|/Game/SpyroContent/CiC_Assets/CiC_Characters/Pony_Soldiers/ABPs/PonySoldier_Shield_ABP.PonySoldier_Shield_ABP_C|Setcoward _aspony_soldier_shield_abp (Variables|Default|Getcoward))
  (Variables|Default|Getmy%20enemy
    (:then
      (Utilities|Time|SetTimerbyFunctionName 0 "enemy check" 1.0 true))
    (:else)))

(event EventTick
  (params (DeltaSeconds :type Float%20%28single-precision%29))
  (|CallParentFunction DeltaSeconds)
  (switch Utilities|FlowControl|Switch|SwitchonAICharacter_States (Variables|/Game/SpyroContent/Global_Assets/Global_Components/Base_AI_Character.Base_AI_Character_C|GetAICharacter_State (Variables|Default|GetWalking_AI_Character))
    (:NewEnumerator0
      (bind _my_enemy (Variables|Default|Getmy%20enemy)
        (:then
          (if (and (not (Utilities|Enum|Equal(Enum) (Variables|/Game/SpyroContent/Global_Assets/Global_Components/Base_AI_Character.Base_AI_Character_C|GetAICharacter_State (Variables|/Game/SpyroContent/Global_Assets/Global_Characters/AI_Characters/Actors/Base_AICharacter_BP.Base_AICharacter_BP_C|GetWalking_AI_Character _my_enemy)) "NewEnumerator3")) (<= (Transformation|GetDistanceTo self) 5.5e+02))
            (Transformation|SetActorRotation (Math|Rotator|Lerp(Rotator) (Transformation|GetActorRotation) (Math|Rotator|MakeRotator 0.0 0.0 (.yaw (Math|Rotator|FindLookatRotation (Transformation|GetActorLocation) (Transformation|GetActorLocation (Variables|Default|Getmy%20enemy))))) (* (Utilities|Time|GetWorldDeltaSeconds) 2e+01) true))))
        (:else)))))

(fn ConstructionScript
  (|CallParentFunction))

(fn EnemyCheck
  (bind _my_enemy (Variables|Default|Getmy%20enemy)
    (:then
      (bind _aspony_soldier_shield_abp (Utilities|Casting|CastToPonySoldier_Shield_ABP (Components|SkeletalMesh|GetAnimInstance (Variables|Character|GetMesh))))
      (Variables|/Game/SpyroContent/CiC_Assets/CiC_Characters/Pony_Soldiers/ABPs/PonySoldier_Shield_ABP.PonySoldier_Shield_ABP_C|Setmy%20enemy%20is%20dead _aspony_soldier_shield_abp (or (Utilities|Enum|Equal(Enum) (Variables|/Game/SpyroContent/Global_Assets/Global_Components/Base_AI_Character.Base_AI_Character_C|GetAICharacter_State (Variables|/Game/SpyroContent/Global_Assets/Global_Characters/AI_Characters/Actors/Base_AICharacter_BP.Base_AICharacter_BP_C|GetWalking_AI_Character _my_enemy)) "NewEnumerator3") (> (Transformation|GetDistanceTo _my_enemy self) (Variables|Default|Getenemy%20distance)))))
    (:else)))