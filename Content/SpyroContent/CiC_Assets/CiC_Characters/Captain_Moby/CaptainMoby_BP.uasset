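; Captain Moby NPC Blueprint that extends a parent talking NPC with player protection and music handling during dialogue.
; While talking, it makes the player invincible, sets their ice and fear death flags, and clears freeze and fear, resetting the flags afterward.
; On UI submit it flags music to stay paused for certain choices in GlobalPersistentLevel.
; When talking finishes, a bound event unpauses music unless WontTalk is set.
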(event Custom|Resume%20Music?
  (if (not (Variables|Default|GetWon't%20Talk))
    (CallFunction|Pause/UnpauseMusic self false false)))

(event EventInvokedUISubmit
  (bind _returnvalue (Game|GetCurrentLevelName true))
  (Variables|Default|SetDont_Unpause_Music_After_Talking (Math|Boolean|ANDBoolean (Utilities|Enum|Equal(Enum) _returnvalue "GlobalPersistentLevel") (> (Variables|Default|GetCurrent_Dialogue_Index) 0) (< (Variables|Default|GetChosen_Choice_Number) 3)))
  (|CallParentFunction))

(event EventBeginPlay
  (|CallParentFunction)
  (EventDispatchers|BindEventtoDoneTalking (delegate Custom|Resume%20Music?)))

(fn ConstructionScript
  (|CallParentFunction))

(fn OnNPCTalkingStart
  (params (Player%20I%20Am%20Talking%20To :type BP%20Base%20Playable%20Object%20Reference))
  (bind _damageable (Variables|/Game/SpyroContent/Global_Assets/Global_Characters/Playable_Characters/BP_Base_Playable.BP_Base_Playable_C|GetDamageable Player%20I%20Am%20Talking%20To))
  (|CallParentFunction Player%20I%20Am%20Talking%20To)
  (Variables|/Game/SpyroContent/Global_Assets/Global_Components/Damageable_Com.Damageable_Com_C|SetInvincible _damageable true)
  (Variables|/Game/SpyroContent/Global_Assets/Global_Components/Damageable_Com.Damageable_Com_C|SetDies_to_Ice _damageable true)
  (Variables|/Game/SpyroContent/Global_Assets/Global_Components/Damageable_Com.Damageable_Com_C|SetDies_to_Fear _damageable true)
  (Default|Melt _damageable)
  (Default|StopBeingAfraid _damageable))

(fn OnNPCTalkingEnd
  (params (Player%20I%20Am%20Talking%20To :type BP%20Base%20Playable%20Object%20Reference))
  (bind _damageable (Variables|/Game/SpyroContent/Global_Assets/Global_Characters/Playable_Characters/BP_Base_Playable.BP_Base_Playable_C|GetDamageable Player%20I%20Am%20Talking%20To))
  (|CallParentFunction Player%20I%20Am%20Talking%20To)
  (Variables|/Game/SpyroContent/Global_Assets/Global_Components/Damageable_Com.Damageable_Com_C|SetInvincible _damageable false)
  (Variables|/Game/SpyroContent/Global_Assets/Global_Components/Damageable_Com.Damageable_Com_C|SetDies_to_Ice _damageable false)
  (Variables|/Game/SpyroContent/Global_Assets/Global_Components/Damageable_Com.Damageable_Com_C|SetDies_to_Fear _damageable false))