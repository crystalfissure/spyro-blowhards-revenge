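; Skybox_Hider is an actor whose mesh, as its name suggests, masks the skybox until it is told to reveal it.
; On BeginPlay it creates a dynamic material instance from Skybox_Hider_Mat and a timeline animates its Opacity parameter.
; UnhideSkybox stops that timeline, animates Opacity with a second timeline, and destroys the actor after a short fixed delay.
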(event Custom|Unhide%20Skybox
  (Utilities|FlowControl|Sequence
    (:then_0
      (bind _newtrack_0 (Timeline|Timeline_0 Stop)
        (:Update
          (Rendering|Material|SetScalarParameterValue (Variables|Default|GetMat%20Inst) "Opacity" _newtrack_0 :!class /Script/Engine.MaterialInstanceDynamic))))
    (:then_1
      (bind _newtrack_0_2 (Timeline|Timeline_1 PlayFromStart)
        (:Update
          (Rendering|Material|SetScalarParameterValue (Variables|Default|GetMat%20Inst) "Opacity" _newtrack_0_2 :!class /Script/Engine.MaterialInstanceDynamic))))
    (:then_2
      (Utilities|FlowControl|Delay 0.6)
      (Actor|DestroyActor))))

(event EventBeginPlay
  (bind _returnvalue (Rendering|Material|CreateDynamicMaterialInstance (Variables|Default|GetStaticMesh) 0 "/Game/SpyroContent/CiC_Assets/CiC_Level_Items/Boat/Materials/Skybox_Hider_Mat.Skybox_Hider_Mat" "None" :!class /Script/Engine.PrimitiveComponent))
  (Variables|Default|SetMat%20Inst _returnvalue)
  (bind _newtrack_0 (Timeline|Timeline_0 PlayFromStart)
    (:Update
      (Rendering|Material|SetScalarParameterValue (Variables|Default|GetMat%20Inst) "Opacity" _newtrack_0 :!class /Script/Engine.MaterialInstanceDynamic))))

(fn ConstructionScript)