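; Multiverse portal Blueprint that shows an open or closed mesh according to the player's saved progress.
; It extends a parent portal's activate and deactivate events, reading the Spyro save data after each parent call.
; Activation sets the open mesh when primary collectibles meet the required count or the levels cheat is on; deactivation sets the closed mesh when neither holds.
; Both swaps happen only when the required count is above zero.
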(event EventActivatePortal?
  (bind _required_primary_collectables (Variables|Default|GetRequired_Primary_Collectables))
  (|CallParentFunction)
  (bind _asspyro_save_data (CallFunction|LoadSpyroGame self))
  (if (and (or (Variables|/Game/SpyroContent/Global_Assets/Global_SaveData/Spyro_SaveData.Spyro_SaveData_C|GetLevels_Cheat _asspyro_save_data) (>= (Variables|/Game/SpyroContent/Global_Assets/Global_SaveData/Spyro_SaveData.Spyro_SaveData_C|GetNumber_of_PrimaryCollectibles _asspyro_save_data) _required_primary_collectables)) (> _required_primary_collectables 0))
    (Components|StaticMesh|SetStaticMesh (Variables|Default|GetStaticMesh) "/Game/SpyroContent/CiC_Assets/CiC_Level_Items/CiC_Portals/multiverse_portal.multiverse_portal")))

(event EventDeactivatePortal?
  (bind _required_primary_collectables (Variables|Default|GetRequired_Primary_Collectables))
  (|CallParentFunction)
  (bind _asspyro_save_data (CallFunction|LoadSpyroGame self))
  (if (Math|Boolean|ANDBoolean (< (Variables|/Game/SpyroContent/Global_Assets/Global_SaveData/Spyro_SaveData.Spyro_SaveData_C|GetNumber_of_PrimaryCollectibles _asspyro_save_data) _required_primary_collectables) (> _required_primary_collectables 0) (not (Variables|/Game/SpyroContent/Global_Assets/Global_SaveData/Spyro_SaveData.Spyro_SaveData_C|GetLevels_Cheat _asspyro_save_data)))
    (Components|StaticMesh|SetStaticMesh (Variables|Default|GetStaticMesh) "/Game/SpyroContent/CiC_Assets/CiC_Level_Items/CiC_Portals/multiverse_portal_closed.multiverse_portal_closed")))

(fn ConstructionScript
  (|CallParentFunction))