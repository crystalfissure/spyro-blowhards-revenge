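; Skin collectable pickup for Spyro, apparently a base class since its ShowMySkin hook is empty.
; Player capsule overlap collects it unless a thief stole it or an NPC awards it; NPC awards auto-collect, then restore camera and input.
; Collection runs once: effects, skin reveal, dust poof, music unpause, destroy.
; A helper checks save data for prior ownership, and the visible skeletal mesh spins on Tick.
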(event OnComponentBeginOverlap(Hitbox)
  (params (OverlappedComponent :type Primitive%20Component%20Object%20Reference) (OtherActor :type Actor%20Object%20Reference) (OtherComp :type Primitive%20Component%20Object%20Reference) (OtherBodyIndex :type Integer) (bFromSweep :type Boolean) (SweepResult :type Hit%20Result%20Structure%20%28by%20ref%29))
  (bind _hitbox (Variables|Default|GetHitbox))
  (bind _hitbox_2 (Variables|Default|GetHitbox))
  (bind _returnvalue (Transformation|GetWorldLocation _hitbox_2))
  (bind _returnvalue_2 (Transformation|GetWorldLocation _hitbox))
  (bind _asbp_base_playable (Utilities|Casting|CastToBP_Base_Playable OtherActor))
  (if (and (== (Variables|/Script/Engine.Character|GetCapsuleComponent _asbp_base_playable) OtherComp) (not (Variables|Default|GetCannot%20Be%20Collected)))
    (Variables|/Game/SpyroContent/Global_Assets/Global_Components/NPC_Award_Item.NPC_Award_Item_C|GetNPC%20Who%20Awarded%20Me (Variables|Default|GetNPC_Award_Item)
      (:then)
      (:else
        (Utilities|FlowControl|DoOnce false
          (:Completed
            (Effects|SpawnEmitteratLocation "/Game/SpyroContent/CiC_Assets/CiC_Level_Items/Dragon_Candle/PS_Fireworks_Burst.PS_Fireworks_Burst" _returnvalue_2)
            (Audio|PlaySoundatLocation "/Game/SpyroContent/Global_Assets/Global_Level_Items/Gems/Audio/gem_collection.gem_collection" _returnvalue_2 "0, 0, 0" 1.0 1.0 0.0 0 0 0)
            (CallFunction|ShowMySkin)
            (Rendering|SetVisibility (Variables|Default|GetStaticMesh) false false)
            (Utilities|FlowControl|Delay 1.5)
            (Effects|SpawnEmitteratLocation "/Game/SpyroContent/Global_Assets/Global_Particles/P_DustCloud.P_DustCloud" _returnvalue "0, 0, 0" "0.500000,0.500000,0.500000")
            (Audio|PlaySoundatLocation "/Game/SpyroContent/Global_Assets/Global_Characters/AI_Characters/death_poof_s1.death_poof_s1" _returnvalue "0, 0, 0" 1.0 1.0 0.0 0 0 0)
            (CallFunction|Pause/UnpauseMusic self false false)
            (Actor|DestroyActor)))))))

(event Custom|Invoked%20Collect
  (bind _hitbox (Variables|Default|GetHitbox))
  (bind _hitbox_2 (Variables|Default|GetHitbox))
  (bind _returnvalue (Transformation|GetWorldLocation _hitbox_2))
  (bind _returnvalue_2 (Transformation|GetWorldLocation _hitbox))
  (Utilities|FlowControl|DoOnce false
    (:Completed
      (Effects|SpawnEmitteratLocation "/Game/SpyroContent/CiC_Assets/CiC_Level_Items/Dragon_Candle/PS_Fireworks_Burst.PS_Fireworks_Burst" _returnvalue_2)
      (Audio|PlaySoundatLocation "/Game/SpyroContent/Global_Assets/Global_Level_Items/Gems/Audio/gem_collection.gem_collection" _returnvalue_2 "0, 0, 0" 1.0 1.0 0.0 0 0 0)
      (CallFunction|ShowMySkin)
      (Rendering|SetVisibility (Variables|Default|GetStaticMesh) false false)
      (Utilities|FlowControl|Delay 1.5)
      (Effects|SpawnEmitteratLocation "/Game/SpyroContent/Global_Assets/Global_Particles/P_DustCloud.P_DustCloud" _returnvalue "0, 0, 0" "0.500000,0.500000,0.500000")
      (Audio|PlaySoundatLocation "/Game/SpyroContent/Global_Assets/Global_Characters/AI_Characters/death_poof_s1.death_poof_s1" _returnvalue "0, 0, 0" 1.0 1.0 0.0 0 0 0)
      (CallFunction|Pause/UnpauseMusic self false false)
      (Actor|DestroyActor))))

(event Custom|On%20Awarded%20by%20NPC
  (Utilities|FlowControl|Delay 1.0)
  (CallFunction|InvokedCollect)
  (bind _player_who_was_awarded_me (Variables|/Game/SpyroContent/Global_Assets/Global_Components/NPC_Award_Item.NPC_Award_Item_C|GetPlayer%20Who%20Was%20Awarded%20Me (Variables|Default|GetNPC_Award_Item))
    (:then
      (Default|HideBlackBars (Variables|/Game/SpyroContent/Global_Assets/Global_Characters/Playable_Characters/BP_Base_Playable.BP_Base_Playable_C|GetSpyroContr_Ref _player_who_was_awarded_me))
      (Game|Player|SetViewTargetwithBlend (Variables|/Game/SpyroContent/Global_Assets/Global_Characters/Playable_Characters/BP_Base_Playable.BP_Base_Playable_C|GetSpyroContr_Ref _player_who_was_awarded_me) _player_who_was_awarded_me 1.0 "VTBlend_Linear" 0.0 false)
      (Utilities|FlowControl|Delay 1.0)
      (bind _player_who_was_awarded_me_2 (Variables|/Game/SpyroContent/Global_Assets/Global_Components/NPC_Award_Item.NPC_Award_Item_C|GetPlayer%20Who%20Was%20Awarded%20Me (Variables|Default|GetNPC_Award_Item))
        (:then
          (Input|EnableInput _player_who_was_awarded_me_2 (Variables|/Game/SpyroContent/Global_Assets/Global_Characters/Playable_Characters/BP_Base_Playable.BP_Base_Playable_C|GetSpyroContr_Ref _player_who_was_awarded_me_2))
          (Variables|/Game/SpyroContent/Global_Assets/Global_Characters/Playable_Characters/BP_Base_Playable.BP_Base_Playable_C|SetDid%20we%20disable%20input? _player_who_was_awarded_me_2 false))
        (:else
          _))
      (bind _npc_who_awarded_me (Variables|/Game/SpyroContent/Global_Assets/Global_Components/NPC_Award_Item.NPC_Award_Item_C|GetNPC%20Who%20Awarded%20Me (Variables|Default|GetNPC_Award_Item))
        (:then
          (if (not (Variables|/Game/SpyroContent/Global_Assets/Global_Characters/NPCs/NPC_Base_BP.NPC_Base_BP_C|GetWon't%20Talk%20A%202nd%20Time _npc_who_awarded_me))
            (Development|SetHiddeninGame (Variables|/Game/SpyroContent/Global_Assets/Global_Characters/NPCs/NPC_Base_BP.NPC_Base_BP_C|GetTriangle_to_Talk_Text _npc_who_awarded_me) false false)))
        (:else)))
    (:else)))

(event Custom|Stolen%20By%20Thief
  (Variables|Default|SetCannot%20Be%20Collected true))

(event EventBeginPlay
  (EventDispatchers|BindEventtoAThiefStoleMe (Variables|Default|GetNPC_Award_Item) (delegate Custom|Stolen%20By%20Thief))
  (EventDispatchers|BindEventtoNPCAwardSpawned (Variables|Default|GetNPC_Award_Item) (delegate Custom|On%20Awarded%20by%20NPC)))

(event EventTick
  (params (DeltaSeconds :type Float%20%28single-precision%29))
  (bind _skeletalmesh (Variables|Default|GetSkeletalMesh))
  (if (Variables|/Script/Engine.SceneComponent|GetbVisible _skeletalmesh)
    (Transformation|AddLocalRotation _skeletalmesh (Math|Rotator|MakeRotator 0.0 0.0 (* DeltaSeconds -2e+02)) false false)))

(fn ConstructionScript)

(fn ShowMySkin)

(fn CheckifWeAlreadyHaveThisSkin
  (bind (_asspyro_save_data _as_persistent_data) (CallFunction|LoadSpyroGame self))
  (Variables|Default|SetYou%20Already%20Have%20This%20Skin (Utilities|Array|Get(acopy) (.itemsplayergot (Utilities|Array|Get(acopy) (.membervar_0 (Utilities|Array|Get(acopy) (Variables|/Game/SpyroContent/Global_Assets/Global_SaveData/Spyro_SaveData.Spyro_SaveData_C|GetLevel_Item_Info _asspyro_save_data) (Variables|/Game/SpyroContent/Global_Assets/Global_SaveData/Spyro_PersistantData.Spyro_PersistantData_C|GetCurrent_Homeworld_Index _as_persistent_data))) (Variables|/Game/SpyroContent/Global_Assets/Global_SaveData/Spyro_PersistantData.Spyro_PersistantData_C|GetCurrent_Level_Index _as_persistent_data))) (Variables|/Game/SpyroContent/Global_Assets/Global_Components/NPC_Award_Item.NPC_Award_Item_C|GetLevel%20Item%20Index (Variables|Default|GetNPC_Award_Item)))))