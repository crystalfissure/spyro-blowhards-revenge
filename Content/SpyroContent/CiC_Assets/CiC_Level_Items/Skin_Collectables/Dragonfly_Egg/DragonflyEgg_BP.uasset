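; Dragonfly egg collectable that unlocks a Sparx skin, extending a parent skin-collectable Blueprint.
; BeginPlay tints the egg through a dynamic material and binds NPCAwardItem thief events: theft plays a held animation, and the thief's death triggers delayed collection.
; ShowMySkin swaps the egg for the idling skin mesh from the current adventure's data and shows a temporary name or already-owned widget.
; It saves the unlock, recording a collectible unless flagged as owned.
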(event Custom|On%20Thief%20Dies
  (Utilities|FlowControl|Delay 2.5)
  (Transformation|SetActorRotation "0, 0, 0")
  (CallFunction|InvokedCollect))

(event Custom|On%20Dragonfly%20Egg%20Stolen
  (Components|Animation|PlayAnimation (Variables|Default|GetDragonflyEggMesh) "/Game/SpyroContent/CiC_Assets/CiC_Level_Items/Skin_Collectables/Dragonfly_Egg/dragonfly_egg_held_by_thief.dragonfly_egg_held_by_thief" true))

(event EventBeginPlay
  (bind _npc_award_item (Variables|Default|GetNPC_Award_Item))
  (|CallParentFunction)
  (bind _returnvalue (Rendering|Material|CreateDynamicMaterialInstance (Variables|Default|GetDragonflyEggMesh) 0 "/Game/SpyroContent/Global_Assets/Global_Materials/Material_Instances/Untex_Vertex_Color.Untex_Vertex_Color" "None" :!class /Script/Engine.PrimitiveComponent))
  (Rendering|Material|SetVectorParameterValue _returnvalue "ColorChange" (Math|Conversions|ToLinearColor(Color) (Variables|Default|GetEgg%20Color)) :!class /Script/Engine.MaterialInstanceDynamic)
  (EventDispatchers|BindEventtoAThiefStoleMe _npc_award_item (delegate Custom|On%20Dragonfly%20Egg%20Stolen))
  (EventDispatchers|BindEventtoMyThiefDied _npc_award_item (delegate Custom|On%20Thief%20Dies)))

(fn ConstructionScript
  (|CallParentFunction))

(fn ShowMySkin
  (bind _skeletalmesh (Variables|Default|GetSkeletalMesh))
  (bind _npc_award_item (Variables|Default|GetNPC_Award_Item))
  (bind _npc_who_awarded_me (Variables|/Game/SpyroContent/Global_Assets/Global_Components/NPC_Award_Item.NPC_Award_Item_C|GetNPC%20Who%20Awarded%20Me _npc_award_item))
  (|CallParentFunction)
  (Rendering|SetVisibility (Variables|Default|GetDragonflyEggMesh) false false)
  (bind (_asspyro_save_data _as_persistent_data _slot_name) (CallFunction|LoadSpyroGame self))
  (Class|SkinnedMeshComponent|SetSkeletalMesh _skeletalmesh (.mesh (Utilities|Array|Get(acopy) (.Sparx_Skins_Struct (Utilities|GetClassDefaults (Variables|/Game/SpyroContent/Global_Assets/Global_SaveData/Spyro_PersistantData.Spyro_PersistantData_C|GetCurrent_AdventureInfo _as_persistent_data))) (Variables|Default|GetMy%20Skin%20Index))) true)
  (Rendering|SetVisibility _skeletalmesh true false)
  (Components|Animation|PlayAnimation _skeletalmesh "/Game/SpyroContent/Global_Assets/Global_Characters/Sparx/Animations/sparx_Anim_Skeletal_Sparx_Skeleton_Sparx_Idle_Skeletal.sparx_Anim_Skeletal_Sparx_Skeleton_Sparx_Idle_Skeletal" true)
  (bind _returnvalue (UserInterface|CreateWidget "/Game/SpyroContent/Global_Assets/Global_UserInterface/Widgets/YouAlreadyHaveThisX.YouAlreadyHaveThisX_C"))
  (Rendering|Components|TextRender|SetText (Variables|/Game/SpyroContent/Global_Assets/Global_UserInterface/Widgets/YouAlreadyHaveThisX.YouAlreadyHaveThisX_C|GetTextBlock_YouAlreadyHaveThisX _returnvalue) (select (Utilities|Array|Get(acopy) (Variables|/Game/SpyroContent/Global_Assets/Global_SaveData/Spyro_SaveData.Spyro_SaveData_C|GetUnlocked_Sparx_Skins _asspyro_save_data) (Variables|Default|GetMy%20Skin%20Index)) "You already have this skin" (Utilities|Text|ToText(String) (.name (Utilities|Array|Get(acopy) (.Sparx_Skins_Struct (Utilities|GetClassDefaults (Variables|/Game/SpyroContent/Global_Assets/Global_SaveData/Spyro_PersistantData.Spyro_PersistantData_C|GetCurrent_AdventureInfo _as_persistent_data))) (Variables|Default|GetMy%20Skin%20Index))))))
  (UserInterface|Viewport|AddtoViewport _returnvalue 0)
  (Utilities|Array|SetArrayElem (Variables|/Game/SpyroContent/Global_Assets/Global_SaveData/Spyro_SaveData.Spyro_SaveData_C|GetUnlocked_Sparx_Skins _asspyro_save_data) (Variables|Default|GetMy%20Skin%20Index) true true)
  (SaveGame|SaveGametoSlot _asspyro_save_data _slot_name)
  (CallFunction|CheckifWeAlreadyHaveThisSkin)
  (if (Variables|Default|GetYou%20Already%20Have%20This%20Skin)
    _
    (else
      (Default|SaveACollectible _as_persistent_data "NewEnumerator5" "" 0.0 (Variables|/Game/SpyroContent/Global_Assets/Global_Components/NPC_Award_Item.NPC_Award_Item_C|GetLevel%20Item%20Index (Variables|Default|GetNPC_Award_Item)) (select (Utilities|IsValid _npc_who_awarded_me) (Variables|/Game/SpyroContent/Global_Assets/Global_Characters/NPCs/NPC_Base_BP.NPC_Base_BP_C|GetSkill%20Level%20Award _npc_who_awarded_me) (Variables|Default|GetSkill%20Level%20Award)))))
  (Default|DelayedSelf-Destruct _returnvalue 1.5))