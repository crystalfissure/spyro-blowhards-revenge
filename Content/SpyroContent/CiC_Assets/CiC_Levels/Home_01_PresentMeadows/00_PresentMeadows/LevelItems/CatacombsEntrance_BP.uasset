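; Breakable wall marking the catacombs entrance in the Present Meadows level.
; It registers its hitbox with a Damageable component and binds a damage event to it.
; When damaged, it confirms the hit, plays a boulder-break sound, then hides itself and drops mesh collision.
; It spawns Basket_Burst_BP to throw cracked-wall shards, then destroys itself after a short delay.
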(event Custom|CustomEvent
  (Default|CallDamageWasSuccessfullyDealt (Variables|Default|GetDamageable))
  (Audio|PlaySoundatLocation "/Game/SpyroContent/CiC_Assets/CiC_Levels/Home_00_PastChasms/00_PastChasms/Level_Items/Begonias/BreakBoulder2.BreakBoulder2" (Transformation|GetActorLocation) "0, 0, 0" 1.0 1.0 0.0 0 0 0)
  (Rendering|SetActorHiddenInGame true)
  (Collision|SetCollisionResponsetoAllChannels (Variables|Default|GetStaticMesh) "ECR_Ignore")
  (bind _returnvalue (Game|SpawnActorfromClass "/Game/SpyroContent/Global_Assets/Global_Level_Items/Treasure_Containers/Basket/Actors/Basket_Burst_BP.Basket_Burst_BP_C" (Transformation|GetActorTransform) "AdjustIfPossibleButAlwaysSpawn" 0 0))
  (Default|ShardBurstAction _returnvalue "/Game/SpyroContent/CiC_Assets/CiC_Levels/Home_00_PastChasms/00_PastChasms/Meshes/cracked_wall_shard_1.cracked_wall_shard_1" "/Game/SpyroContent/CiC_Assets/CiC_Levels/Home_00_PastChasms/00_PastChasms/Meshes/cracked_wall_shard_2.cracked_wall_shard_2")
  (Utilities|FlowControl|Delay 0.2)
  (Actor|DestroyActor))

(event EventBeginPlay
  (Variables|/Game/SpyroContent/Global_Assets/Global_Components/Damageable_Com.Damageable_Com_C|SetObject's%20Hitbox%20Component (Variables|Default|GetDamageable) (Variables|Default|Gethitbox))
  (EventDispatchers|BindEventtoCallDealDamage (Variables|Default|GetDamageable) (delegate Custom|CustomEvent)))

(fn ConstructionScript
  (|CallParentFunction))