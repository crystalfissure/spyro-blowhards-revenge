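; Headbash_Trigger_BP is an invisible-or-placed trigger in the Present Meadows level that, as its name indicates, responds to a headbash by destroying itself.
; Its Box serves as the Damageable component's hitbox, and a bound event accepts only one specific damage type.
; A playable character's capsule overlapping the Box in a specific player state takes the same path, reporting successful damage before destroying the actor.
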(event OnComponentBeginOverlap(Box)
  (params (OverlappedComponent :type Primitive%20Component%20Object%20Reference) (OtherActor :type Actor%20Object%20Reference) (OtherComp :type Primitive%20Component%20Object%20Reference) (OtherBodyIndex :type Integer) (bFromSweep :type Boolean) (SweepResult :type Hit%20Result%20Structure%20%28by%20ref%29))
  (bind _asbp_base_playable (Utilities|Casting|CastToBP_Base_Playable OtherActor))
  (if (and (== (Variables|/Script/Engine.Character|GetCapsuleComponent _asbp_base_playable) OtherComp) (Utilities|Enum|Equal(Enum) (Variables|/Game/SpyroContent/Global_Assets/Global_Characters/Playable_Characters/BP_Base_Playable.BP_Base_Playable_C|GetPlayer_State _asbp_base_playable) "NewEnumerator8"))
    (Default|CallDamageWasSuccessfullyDealt (Variables|Default|GetDamageable))
    (Actor|DestroyActor)))

(event Custom|CustomEvent_0
  (if (Utilities|Enum|Equal(Enum) (Variables|/Game/SpyroContent/Global_Assets/Global_Components/Damageable_Com.Damageable_Com_C|GetDeal%20Damage%20-%20Damage%20Type (Variables|Default|GetDamageable)) "NewEnumerator2")
    (Default|CallDamageWasSuccessfullyDealt (Variables|Default|GetDamageable))
    (Actor|DestroyActor)))

(event EventBeginPlay
  (Variables|/Game/SpyroContent/Global_Assets/Global_Components/Damageable_Com.Damageable_Com_C|SetObject's%20Hitbox%20Component (Variables|Default|GetDamageable) (Variables|Default|GetBox))
  (EventDispatchers|BindEventtoCallDealDamage (Variables|Default|GetDamageable) (delegate Custom|CustomEvent_0)))

(fn ConstructionScript)