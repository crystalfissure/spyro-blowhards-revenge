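; Harp in Astral Utopia that turns happy when hit, brightening its material, playing a random chirp and showing the happy-harp count on the quest HUD.
; Unless permanently happy, a looping timer counts down, pausing during NPC dialogue, then saddens and dims it and updates the count.
; Player respawn zeroes the countdown and destroys all moving bubbles.
; The count scans every harp's Anim Blueprint IsHappy flag, which holds the mood.
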(event Custom|Harp%20Damaged
  (bind _dynmat (Variables|Default|GetDynMat))
  (bind _asharp_abp (Utilities|Casting|CastToHarp_ABP (Components|SkeletalMesh|GetAnimInstance (Variables|Character|GetMesh))))
  (if (Variables|/Game/SpyroContent/CiC_Assets/CiC_Levels/Home_01_PresentMeadows/01_AstralUtopia/Actors/Harps/Harp_ABP.Harp_ABP_C|GetisHappy _asharp_abp)
    _
    (else
      (Variables|/Game/SpyroContent/CiC_Assets/CiC_Levels/Home_01_PresentMeadows/01_AstralUtopia/Actors/Harps/Harp_ABP.Harp_ABP_C|SetisHappy _asharp_abp true)
      (if (Variables|Default|Getpermanently%20happy)
        _
        (else
          (bind _asspyro_player_controller (Utilities|Casting|CastToSpyro_PlayerController (Game|GetPlayerController 0))
            (:then
              (bind _total_number_of_happy_harps (CallFunction|GetNumberOfHappyHarps))
              (Default|ShowBottomRightQuestHUD _asspyro_player_controller "/Game/SpyroContent/CiC_Assets/CiC_Levels/Home_01_PresentMeadows/01_AstralUtopia/Actors/Harps/Harp_Flipbook_Mat.Harp_Flipbook_Mat" (Utilities|String|ToString(Integer) _total_number_of_happy_harps) (Variables|Default|GetMax%20Number%20Of%20Quest%20Items)))
            (:CastFailed
              _))))
      (Audio|PlaySoundatLocation (Utilities|Select :Index (Math|Random|RandomIntegerinRange 0 3) :Option%200 "/Game/SpyroContent/CiC_Assets/CiC_Levels/Home_01_PresentMeadows/01_AstralUtopia/Actors/Harps/baby_chirp.baby_chirp" :Option%201 "/Game/SpyroContent/CiC_Assets/CiC_Levels/Home_01_PresentMeadows/01_AstralUtopia/Actors/Harps/baby_chirp_2.baby_chirp_2" :Option%202 "/Game/SpyroContent/CiC_Assets/CiC_Levels/Home_01_PresentMeadows/01_AstralUtopia/Actors/Harps/baby_chirp_3.baby_chirp_3" :Option%203 "/Game/SpyroContent/CiC_Assets/CiC_Levels/Home_01_PresentMeadows/01_AstralUtopia/Actors/Harps/baby_chirp_4.baby_chirp_4") (Transformation|GetActorLocation) "0, 0, 0" 1.7 1.0 0.0 "/Game/SpyroContent/Global_Assets/Global_Audio/Attenuation/Spyro_Attenuation_MediumHigh.Spyro_Attenuation_MediumHigh" 0 0)
      (Development|PrintString "play sound!!!!!")))
  (Utilities|IsValid _dynmat
    (:Is%20Valid
      (Rendering|Material|SetScalarParameterValue _dynmat "Brightness" 1.0 :!class /Script/Engine.MaterialInstanceDynamic))
    (:Is%20Not%20Valid
      _))
  (if (not (Variables|Default|Getpermanently%20happy))
    (Variables|Default|SetSadness%20Countdown 50)
    (Utilities|Time|ClearandInvalidateTimerbyHandle (Variables|Default|GetSadness%20Timer))
    (bind _returnvalue (Utilities|Time|SetTimerbyFunctionName 0 "Countdown to Sadness" 1.0 true))
    (Variables|Default|SetSadness%20Timer _returnvalue)))

(event Custom|when%20player%20dies,%20become%20sad
  (bind _outactors (Actor|GetAllActorsOfClass "/Game/SpyroContent/Global_Assets/Global_Level_Items/Bubble/Bubble_Moving_BP.Bubble_Moving_BP_C"))
  (for _array_element _outactors
    (Actor|DestroyActor _array_element))
  (Variables|Default|SetSadness%20Countdown 0)
  (Development|PrintString "HARP SAD U DIED"))

(event EventBeginPlay
  (|CallParentFunction)
  (Variables|/Game/SpyroContent/Global_Assets/Global_Components/Damageable_Com.Damageable_Com_C|SetObject's%20Hitbox%20Component (Variables|Default|GetDamageable) (Variables|Default|Gethitbox))
  (bind _returnvalue (Rendering|Material|CreateDynamicMaterialInstance (Variables|Character|GetMesh) 0 (Rendering|Material|GetMaterial (Variables|Character|GetMesh) 0) "None" :!class /Script/Engine.PrimitiveComponent))
  (bind _output_get (Variables|Default|SetDynMat _returnvalue))
  (Rendering|Material|SetScalarParameterValue _output_get "Brightness" 0.25 :!class /Script/Engine.MaterialInstanceDynamic)
  (EventDispatchers|BindEventtoCallDealDamage (Variables|Default|GetDamageable) (delegate Custom|Harp%20Damaged))
  (bind _asspyro_persistant_data (Utilities|Casting|CastToSpyro_PersistantData (Game|GetGameInstance)))
  (EventDispatchers|BindEventtoAnyPlayerIsAbouttoRespawn _asspyro_persistant_data (delegate Custom|when%20player%20dies,%20become%20sad)))

(event EventResetThisAICharacter)

(fn ConstructionScript
  (|CallParentFunction))

(fn CountdowntoSadness
  (if (Variables|Default|Getpermanently%20happy)
    (Utilities|Time|ClearandInvalidateTimerbyHandle (Variables|Default|GetSadness%20Timer))
    (else
      (bind _asbp_base_playable (Utilities|Casting|CastToBP_Base_Playable (Game|GetPlayerCharacter 0))
        (:then
          (Variables|/Game/SpyroContent/Global_Assets/Global_Characters/Playable_Characters/BP_Base_Playable.BP_Base_Playable_C|GetTalking_NPC _asbp_base_playable
            (:then)
            (:else
              _)))
        (:CastFailed
          _))
      (bind _output_get (Variables|Default|SetSadness%20Countdown (select (> (- (Variables|Default|GetSadness%20Countdown) 1) 0) (- (Variables|Default|GetSadness%20Countdown) 1) 0)))
      (if (<= _output_get 0)
        (bind _asharp_abp (Utilities|Casting|CastToHarp_ABP (Components|SkeletalMesh|GetAnimInstance (Variables|Character|GetMesh)))
          (:then
            (Variables|/Game/SpyroContent/CiC_Assets/CiC_Levels/Home_01_PresentMeadows/01_AstralUtopia/Actors/Harps/Harp_ABP.Harp_ABP_C|SetisHappy _asharp_abp false)
            (bind _asspyro_player_controller (Utilities|Casting|CastToSpyro_PlayerController (Game|GetPlayerController 0))
              (:then
                (bind _total_number_of_happy_harps (CallFunction|GetNumberOfHappyHarps))
                (Rendering|Components|TextRender|SetText (Variables|/Game/SpyroContent/Global_Assets/Global_UserInterface/Widgets/HUD.HUD_C|GetQuestItem_TextBlock_BottomRight (Variables|/Game/SpyroContent/Global_Assets/Global_Characters/Playable_Characters/Spyro_PlayerController.Spyro_PlayerController_C|GetMy_HUD_Ref _asspyro_player_controller)) (Utilities|Text|ToText(String) (Utilities|String|Append (Utilities|String|ToString(Integer) _total_number_of_happy_harps) "/" (Variables|Default|GetMax%20Number%20of%20Quest%20Items)))))
              (:CastFailed
                _)))
          (:CastFailed
            _))
        (Rendering|Material|SetScalarParameterValue (Variables|Default|GetDynMat) "Brightness" 0.5 :!class /Script/Engine.MaterialInstanceDynamic)
        (Utilities|Time|ClearandInvalidateTimerbyHandle (Variables|Default|GetSadness%20Timer))))))

(fn GetNumberOfHappyHarps
  (LocalVariables|SetNumber%20of%20Happy%20Harps 0)
  (bind _outactors (Actor|GetAllActorsOfClass "Harp_BP_C"))
  (for _array_element _outactors
    (bind _asharp_abp (Utilities|Casting|CastToHarp_ABP (Components|SkeletalMesh|GetAnimInstance (Variables|/Script/Engine.Character|GetMesh _array_element))))
    (if (Variables|/Game/SpyroContent/CiC_Assets/CiC_Levels/Home_01_PresentMeadows/01_AstralUtopia/Actors/Harps/Harp_ABP.Harp_ABP_C|GetisHappy _asharp_abp)
      (Math|Integer|IncrementInt (LocalVariables|GetNumber%20of%20Happy%20Harps))))
  (return (LocalVariables|GetNumber%20of%20Happy%20Harps)))