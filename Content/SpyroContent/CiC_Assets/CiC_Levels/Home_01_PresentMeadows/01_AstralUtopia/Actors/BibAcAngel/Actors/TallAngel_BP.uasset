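; TallAngel_BP is the tall variant of an Angel AI character in the Astral Utopia level, extending a parent Blueprint.
; On each state change it runs the parent logic, then points the Damageable hitbox at the angel's head.
; When the state is Dying, it spawns a Basket_Burst_BP at each of its five character meshes, bursting them into angel shards.
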(event EventAngelStateChanged
  (|CallParentFunction)
  (Variables|/Game/SpyroContent/Global_Assets/Global_Components/Damageable_Com.Damageable_Com_C|SetObject's%20Hitbox%20Component (Variables|Default|GetDamageable) (Variables|Default|Getangels_hitbox_head))
  (switch Utilities|FlowControl|Switch|SwitchonAICharacter_States (Variables|/Game/SpyroContent/Global_Assets/Global_Components/Base_AI_Character.Base_AI_Character_C|GetAICharacter_State (Variables|Default|GetWalking_AI_Character))
    (:NewEnumerator3
      (for _array_element (Utilities|Array|MakeArray (Variables|Default|GetCharacterMesh1) (Variables|Default|GetCharacterMesh2) (Variables|Default|GetCharacterMesh3) (Variables|Default|GetCharacterMesh4) (Variables|Default|GetCharacterMesh5))
        (bind _returnvalue (Game|SpawnActorfromClass "/Game/SpyroContent/Global_Assets/Global_Level_Items/Treasure_Containers/Basket/Actors/Basket_Burst_BP.Basket_Burst_BP_C" (Math|Transform|MakeTransform (Transformation|GetWorldLocation _array_element) "0, 0, 0" "1,1,1") "AlwaysSpawn" 0 0))
        (Default|ShardBurstAction _returnvalue "/Game/SpyroContent/CiC_Assets/CiC_Levels/Home_01_PresentMeadows/01_AstralUtopia/Actors/BibAcAngel/StMsh/angel_shard_1.angel_shard_1" "/Game/SpyroContent/CiC_Assets/CiC_Levels/Home_01_PresentMeadows/01_AstralUtopia/Actors/BibAcAngel/StMsh/angel_shard_2.angel_shard_2")))))

(fn ConstructionScript
  (|CallParentFunction))