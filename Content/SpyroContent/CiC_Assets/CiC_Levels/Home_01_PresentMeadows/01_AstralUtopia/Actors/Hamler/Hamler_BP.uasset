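; Hamler creature for the Astral Utopia level, a swallowable, spittable object that burns and resets when it hits lava.
; BeginPlay makes dynamic material instances so the body can be tinted.
; A HotLava_BP collision hit plays the burnt animation and sounds, darkens the materials and changes its swallow/spit state.
; After a delayed poof, it restores idle animation and color, calls the inherited reset, then re-arms the DoOnce guard.
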(event OnComponentHit(COL)
  (params (HitComponent :type Primitive%20Component%20Object%20Reference) (OtherActor :type Actor%20Object%20Reference) (OtherComp :type Primitive%20Component%20Object%20Reference) (NormalImpulse :type Vector :default "0, 0, 0") (Hit :type Hit%20Result%20Structure%20%28by%20ref%29))
  (bind _returnvalue (Transformation|GetActorLocation))
  (bind _returnvalue_2 (Transformation|GetActorLocation))
  (bind _ashot_lava_bp (Utilities|Casting|CastToHotLava_BP OtherActor))
  (if (== (Variables|/Game/SpyroContent/Global_Assets/Global_Level_Items/HotLava/HotLava_BP.HotLava_BP_C|GetCollision _ashot_lava_bp) OtherComp)
    (Utilities|FlowControl|DoOnce false
      (:Completed
        (Components|Animation|PlayAnimation (Variables|Default|GetSkeletalMesh) "/Game/SpyroContent/CiC_Assets/CiC_Levels/Home_01_PresentMeadows/01_AstralUtopia/Actors/Hamler/celestial_hamlet_Anim_Armature_Burnt.celestial_hamlet_Anim_Armature_Burnt" false)
        (CallFunction|GotoIdleSwallowableState true)
        (Variables|Default|SetSpittable%20Object%20State "NewEnumerator1")
        (for _array_element (Variables|Default|GetDynMatRefs)
          (Rendering|Material|SetVectorParameterValue _array_element "ColorChange" "(R=0.020833,G=0.020833,B=0.020833,A=1.000000)" :!class /Script/Engine.MaterialInstanceDynamic))
        (Audio|PlaySoundatLocation "/Game/SpyroContent/Global_Assets/Global_Characters/Playable_Characters/Spyro/Audio/spyro_burnt_butt.spyro_burnt_butt" _returnvalue_2 "0, 0, 0" 1.0 1.0 0.0 "/Game/SpyroContent/Global_Assets/Global_Audio/Attenuation/Spyro_Attenuation_Absolute_Farthest.Spyro_Attenuation_Absolute_Farthest" 0 0)
        (Utilities|FlowControl|Delay 1.0)
        (Audio|PlaySoundatLocation "/Game/SpyroContent/Global_Assets/Global_Characters/Playable_Characters/Spyro/Audio/spyro_burnt_death_flop.spyro_burnt_death_flop" _returnvalue_2 "0, 0, 0" 1.0 1.0 0.0 "/Game/SpyroContent/Global_Assets/Global_Audio/Attenuation/Spyro_Attenuation_Absolute_Farthest.Spyro_Attenuation_Absolute_Farthest" 0 0)
        (Utilities|FlowControl|Delay 1.0)
        (Effects|SpawnEmitteratLocation "/Game/SpyroContent/Global_Assets/Global_Particles/P_DustCloud.P_DustCloud" _returnvalue)
        (Audio|PlaySoundatLocation "/Game/SpyroContent/Global_Assets/Global_Characters/AI_Characters/death_poof_s1.death_poof_s1" _returnvalue "0, 0, 0" 1.0 1.0 0.0 0 0 0)
        (Components|Animation|PlayAnimation (Variables|Default|GetSkeletalMesh) "/Game/SpyroContent/CiC_Assets/CiC_Levels/Home_01_PresentMeadows/01_AstralUtopia/Actors/Hamler/celestial_hamlet_Anim_Armature_Idle.celestial_hamlet_Anim_Armature_Idle" true)
        (for _array_element_2 (Variables|Default|GetDynMatRefs)
          (Rendering|Material|SetVectorParameterValue _array_element_2 "ColorChange" "(R=1.000000,G=1.000000,B=1.000000,A=1.000000)" :!class /Script/Engine.MaterialInstanceDynamic))
        (CallFunction|ResetSpittableObject)
        (Utilities|FlowControl|Delay 0.2)
        (CallFunction|ResetLavaDeath)))))

(event Custom|reset%20lava%20death
  (bind _returnvalue (Transformation|GetActorLocation))
  (bind _returnvalue_2 (Transformation|GetActorLocation))
  (Utilities|FlowControl|DoOnce false) ; enters at Reset
)

(event EventBeginPlay
  (bind _skeletalmesh (Variables|Default|GetSkeletalMesh))
  (|CallParentFunction)
  (for (_array_element _array_index) (Rendering|Material|GetMaterials _skeletalmesh)
    (bind _returnvalue (Rendering|Material|CreateDynamicMaterialInstance _skeletalmesh _array_index _array_element "None" :!class /Script/Engine.PrimitiveComponent))
    (Utilities|Array|AddUnique (Variables|Default|GetDynMatRefs) _returnvalue)))

(fn ConstructionScript
  (|CallParentFunction))