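; Pony angel enemy for the Astral Utopia level that looks angelic while idle or alert and turns into a devil otherwise.
; A looping timer checks the walking AI state and swaps mesh and materials with a bell and dust puff, unless frozen or fear-paralyzed.
; State changes mirror to the flying AI component and remove gravity until death.
; Melting or recovering from fear halts movement.
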(event Custom|angel%20state%20changed
  (bind _walking_ai_character (Variables|Default|GetWalking_AI_Character))
  (bind _charactermovement (Variables|Character|GetCharacterMovement))
  (bind _aicharacter_state (Variables|/Game/SpyroContent/Global_Assets/Global_Components/Base_AI_Character.Base_AI_Character_C|GetAICharacter_State _walking_ai_character))
  (Default|ChangeAICharacterState (Variables|Default|GetFlying_AI_Character) _aicharacter_state)
  (switch Utilities|FlowControl|Switch|SwitchonAICharacter_States _aicharacter_state
    (:NewEnumerator0
      (Variables|/Script/Engine.CharacterMovementComponent|SetGravityScale _charactermovement 0.0 :!label _label))
    (:NewEnumerator1
      (goto _label))
    (:NewEnumerator2
      (goto _label))
    (:NewEnumerator3
      (Variables|/Script/Engine.CharacterMovementComponent|SetGravityScale _charactermovement 1.5))))

(event Custom|Pony%20Angel%20Melted
  (Components|Movement|StopMovementImmediately (Variables|Character|GetCharacterMovement)))

(event EventBeginPlay
  (|CallParentFunction)
  (EventDispatchers|BindEventtoMyStateChanged (Variables|Default|GetWalking_AI_Character) (delegate Custom|angel%20state%20changed))
  (Utilities|Time|SetTimerbyFunctionName 0 "Check for Devil" 0.2 true)
  (EventDispatchers|BindEventtoMeltedfromIce (Variables|Default|GetDamageable) (delegate Custom|Pony%20Angel%20Melted))
  (EventDispatchers|BindEventtoCallStopBeingAfraid (Variables|Default|GetDamageable) (delegate Custom|Pony%20Angel%20Melted)))

(fn ConstructionScript
  (|CallParentFunction))

(fn CheckforDevil
  (bind _returnvalue (Transformation|GetActorLocation))
  (bind _walking_ai_character (Variables|Default|GetWalking_AI_Character))
  (bind _damageable (Variables|Default|GetDamageable))
  (bind _damageable_2 (Variables|Default|GetDamageable))
  (bind _aicharacter_state (Variables|/Game/SpyroContent/Global_Assets/Global_Components/Base_AI_Character.Base_AI_Character_C|GetAICharacter_State _walking_ai_character))
  (if (or (Utilities|Enum|Equal(Enum) _aicharacter_state "NewEnumerator0") (Utilities|Enum|Equal(Enum) _aicharacter_state "NewEnumerator1"))
    (if (Variables|Default|GetAngel%20Mode)
      _
      (else
        (Variables|Default|SetAngel%20Mode true)))
    (if (Math|Boolean|ANDBoolean (not (== (Variables|/Script/Engine.SkinnedMeshComponent|GetSkeletalMesh (Variables|Character|GetMesh)) "/Game/SpyroContent/CiC_Assets/CiC_Levels/Home_01_PresentMeadows/01_AstralUtopia/Actors/PonyAngels/Meshes/pony_soldier_angel.pony_soldier_angel")) (not (Variables|/Game/SpyroContent/Global_Assets/Global_Components/Damageable_Com.Damageable_Com_C|GetFrozen _damageable)) (not (Variables|/Game/SpyroContent/Global_Assets/Global_Components/Damageable_Com.Damageable_Com_C|GetParalyzed_by_Fear _damageable)))
      (Class|SkinnedMeshComponent|SetSkeletalMesh (Variables|Character|GetMesh) "/Game/SpyroContent/CiC_Assets/CiC_Levels/Home_01_PresentMeadows/01_AstralUtopia/Actors/PonyAngels/Meshes/pony_soldier_angel.pony_soldier_angel" false)
      (|fixangelmats)
      (Audio|PlaySoundatLocation "/Game/SpyroContent/CiC_Assets/CiC_Levels/Home_01_PresentMeadows/01_AstralUtopia/Actors/PonyAngels/Audio/Bell1-1.Bell1-1" _returnvalue "0, 0, 0" 0.2 1.0 0.0 "/Game/SpyroContent/Global_Assets/Global_Audio/Attenuation/Spyro_Attenuation_Farther.Spyro_Attenuation_Farther" 0 0)
      (bind _returnvalue_2 (Effects|SpawnEmitteratLocation "/Game/SpyroContent/Global_Assets/Global_Particles/P_DustCloud.P_DustCloud" _returnvalue "0, 0, 0" "1.500000,1.500000,1.500000" :!label _label))
      (Variables|/Script/Engine.ParticleSystemComponent|SetCustomTimeDilation _returnvalue_2 6.0))
    (else
      (if (Variables|Default|GetAngel%20Mode)
        (Variables|Default|SetAngel%20Mode false))
      (if (Math|Boolean|ANDBoolean (not (== (Variables|/Script/Engine.SkinnedMeshComponent|GetSkeletalMesh (Variables|Character|GetMesh)) "/Game/SpyroContent/CiC_Assets/CiC_Levels/Home_01_PresentMeadows/01_AstralUtopia/Actors/PonyAngels/Meshes/pony_soldier_devil.pony_soldier_devil")) (not (Variables|/Game/SpyroContent/Global_Assets/Global_Components/Damageable_Com.Damageable_Com_C|GetFrozen _damageable_2)) (not (Variables|/Game/SpyroContent/Global_Assets/Global_Components/Damageable_Com.Damageable_Com_C|GetParalyzed_by_Fear _damageable_2)))
        (Class|SkinnedMeshComponent|SetSkeletalMesh (Variables|Character|GetMesh) "/Game/SpyroContent/CiC_Assets/CiC_Levels/Home_01_PresentMeadows/01_AstralUtopia/Actors/PonyAngels/Meshes/pony_soldier_devil.pony_soldier_devil" false)
        (|fixdevilmats)
        (Audio|PlaySoundatLocation "/Game/SpyroContent/CiC_Assets/CiC_Levels/Home_01_PresentMeadows/01_AstralUtopia/Actors/PonyAngels/Audio/Bell1-1.Bell1-1" _returnvalue "0, 0, 0" 0.2 0.6 0.0 "/Game/SpyroContent/Global_Assets/Global_Audio/Attenuation/Spyro_Attenuation_Even_Farther.Spyro_Attenuation_Even_Farther" 0 0)
        (goto _label)))))