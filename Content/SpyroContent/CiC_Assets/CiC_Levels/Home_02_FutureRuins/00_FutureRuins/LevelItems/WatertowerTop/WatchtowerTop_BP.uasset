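; Destructible watchtower top for Future Ruins that watches the player and shoots superflames as a quest target.
; Tick turns the capsule toward a playable character, while a looping timer fires at players inside FireballRadius, skipping those talking to NPCs.
; Saved or dynamic skill-based difficulty sets fire rate and radius; Easy disables shooting.
; Destruction plays blast effects, flags whether it was the last watchtower, and shows the destroyed count on the quest HUD.
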(event OnComponentBeginOverlap(FireballRadius)
  (params (OverlappedComponent :type Primitive%20Component%20Object%20Reference) (OtherActor :type Actor%20Object%20Reference) (OtherComp :type Primitive%20Component%20Object%20Reference) (OtherBodyIndex :type Integer) (bFromSweep :type Boolean) (SweepResult :type Hit%20Result%20Structure%20%28by%20ref%29))
  (bind _asbp_base_playable (Utilities|Casting|CastToBP_Base_Playable OtherActor))
  (if (== (Variables|/Script/Engine.Character|GetCapsuleComponent _asbp_base_playable) OtherComp)
    (Utilities|Array|AddUnique (Variables|Default|GetPlayers%20in%20My%20Range) _asbp_base_playable)))

(event OnComponentEndOverlap(FireballRadius)
  (params (OverlappedComponent :type Primitive%20Component%20Object%20Reference) (OtherActor :type Actor%20Object%20Reference) (OtherComp :type Primitive%20Component%20Object%20Reference) (OtherBodyIndex :type Integer))
  (bind _asbp_base_playable (Utilities|Casting|CastToBP_Base_Playable OtherActor))
  (if (== (Variables|/Script/Engine.Character|GetCapsuleComponent _asbp_base_playable) OtherComp)
    (Utilities|Array|RemoveItem (Variables|Default|GetPlayers%20in%20My%20Range) _asbp_base_playable)))

(event Custom|Set%20My%20Difficulty
  (bind _medium_sphere_radius (Variables|Difficulty|GetMedium%20Sphere%20Radius))
  (bind _asspyro_universal_save_data (CallFunction|LoadUniversalSave))
  (if (Utilities|Enum|Equal(Enum) (Variables|/Game/SpyroContent/Global_Assets/Global_SaveData/Spyro_Universal_Save_Data.Spyro_Universal_Save_Data_C|GetDifficulty _asspyro_universal_save_data) "NewEnumerator4")
    (bind _asspyro_save_data (CallFunction|LoadSpyroGame self))
    (bind _difficulty (CallFunction|ConvertSkillLevelFloattoEnum (Variables|/Game/SpyroContent/Global_Assets/Global_SaveData/Spyro_SaveData.Spyro_SaveData_C|GetSkill_Level _asspyro_save_data)))
    (Variables|Difficulty|SetMy%20Current%20Difficulty _difficulty)
    (else
      (Variables|Difficulty|SetMy%20Current%20Difficulty (Variables|/Game/SpyroContent/Global_Assets/Global_SaveData/Spyro_Universal_Save_Data.Spyro_Universal_Save_Data_C|GetDifficulty _asspyro_universal_save_data))))
  (Utilities|Time|ClearandInvalidateTimerbyHandle (Variables|Default|GetFireball%20Timer))
  (bind _returnvalue (Utilities|Time|SetTimerbyFunctionName 0 "Shoot Fireball" (Utilities|Select :Index (Variables|Difficulty|GetMy%20Current%20Difficulty) :NewEnumerator4 1.5 :NewEnumerator0 1.5 :NewEnumerator1 1.5 :NewEnumerator2 1.0 :NewEnumerator3 0.5) true))
  (Variables|Default|SetFireball%20Timer _returnvalue)
  (Components|Sphere|SetSphereRadius (Variables|Default|GetFireball%20Radius) (Utilities|Select :Index (Variables|Difficulty|GetMy%20Current%20Difficulty) :NewEnumerator4 _medium_sphere_radius :NewEnumerator0 _medium_sphere_radius :NewEnumerator1 _medium_sphere_radius :NewEnumerator2 _medium_sphere_radius :NewEnumerator3 (* _medium_sphere_radius 1.5)) true))

(event EventResetThisContainer
  (|CallParentFunction)
  (bind _asspyro_player_controller (Utilities|Casting|CastToSpyro_PlayerController (Game|GetPlayerController 0)))
  (bind _total_number_destroyed (CallFunction|CountWatchtowerTops))
  (Rendering|Components|TextRender|SetText (Variables|/Game/SpyroContent/Global_Assets/Global_UserInterface/Widgets/HUD.HUD_C|GetQuestItem_TextBlock_TopRight (Variables|/Game/SpyroContent/Global_Assets/Global_Characters/Playable_Characters/Spyro_PlayerController.Spyro_PlayerController_C|GetMy_HUD_Ref _asspyro_player_controller)) (Utilities|Text|ToText(String) (Utilities|String|Append (Utilities|String|ToString(Integer) _total_number_destroyed) "/" "6"))))

(event EventBeginPlay
  (|CallParentFunction)
  (Variables|Difficulty|SetMedium%20Sphere%20Radius (Variables|/Script/Engine.SphereComponent|GetSphereRadius (Variables|Default|GetFireball%20Radius)))
  (bind _asspyro_persistant_data (Utilities|Casting|CastToSpyro_PersistantData (Game|GetGameInstance))
    (:then
      (EventDispatchers|BindEventtoDifficultyChanged _asspyro_persistant_data (delegate Custom|Set%20My%20Difficulty)))
    (:CastFailed
      _))
  (CallFunction|SetMyDifficulty))

(event EventTick
  (params (DeltaSeconds :type Float%20%28single-precision%29))
  (if (not (Variables|Default|GetContainer_Destroyed))
    (Variables|Default|GetWatch_Target
      (:then
        (Transformation|SetWorldRotation (Variables|Default|GetCapsule%20Component) (Math|Rotator|FindLookatRotation (Transformation|GetActorLocation) (Transformation|GetActorLocation (Variables|Default|GetWatch_Target))) false false))
      (:else
        (Utilities|FlowControl|DoOnce false :!label _label
          (:Completed
            (Utilities|FlowControl|Delay 1.0)
            (bind _outactors (Actor|GetAllActorsOfClass "/Game/SpyroContent/Global_Assets/Global_Characters/Playable_Characters/BP_Base_Playable.BP_Base_Playable_C"))
            (Utilities|IsValid (Utilities|Array|Get(acopy) _outactors)
              (:Is%20Valid
                (Variables|Default|SetWatch_Target (Utilities|Array|Get(acopy) _outactors))
                (goto _label Reset)))))))))

(event EventTreasureContainerSuccessfullyDamaged
  (bind _returnvalue (Transformation|GetActorLocation))
  (bind _returnvalue_2 (Transformation|GetActorLocation))
  (|CallParentFunction)
  (Variables|Default|SetIm_The_Last_Watchtower_Destroyed true)
  (bind _outactors (Actor|GetAllActorsOfClass "/Game/SpyroContent/CiC_Assets/CiC_Levels/Home_02_FutureRuins/00_FutureRuins/LevelItems/WatchtowerBase/WatchtowerBase_BP.WatchtowerBase_BP_C"))
  (bind _array_element (Utilities|Array|ForEachLoopwithBreak _outactors)
    (:LoopBody
      (if (and (not (== _array_element self)) (not (Variables|/Game/SpyroContent/Global_Assets/Global_Level_Items/Treasure_Containers/Treasure_Container_Base_BP.Treasure_Container_Base_BP_C|GetContainer_Destroyed _array_element)))
        (Variables|Default|SetIm_The_Last_Watchtower_Destroyed false)))
    (:Completed
      (Audio|PlaySoundatLocation "/Game/SpyroContent/Global_Assets/Global_Level_Items/Treasure_Containers/Balloon_Vase/Audio/balloon_pop.balloon_pop" _returnvalue "0, 0, 0" 2.0 0.8 0.0 "/Game/SpyroContent/Global_Assets/Global_Audio/Attenuation/Spyro_Attenuation_The_Absolute_Farthest.Spyro_Attenuation_The_Absolute_Farthest" 0 0)
      (Audio|PlaySoundatLocation "/Game/SpyroContent/Global_Assets/Global_Level_Items/Superflame/Audio/underwater_superflame_sound.underwater_superflame_sound" _returnvalue "0, 0, 0" 2.0 0.8 0.0 "/Game/SpyroContent/Global_Assets/Global_Audio/Attenuation/Spyro_Attenuation_The_Absolute_Farthest.Spyro_Attenuation_The_Absolute_Farthest" 0 0)
      (Effects|SpawnEmitteratLocation "/Game/SpyroContent/Global_Assets/Global_Level_Items/Superflame/Particles/Superflame_Blast.Superflame_Blast" (Math|Vector|MakeVector (.x _returnvalue_2) (.y _returnvalue_2) (+ (.z _returnvalue_2) 1e+02)) "0, 0, 0" "5.000000,5.000000,5.000000")
      (bind _asspyro_player_controller (Utilities|Casting|CastToSpyro_PlayerController (Game|GetPlayerController 0)))
      (bind _total_number_destroyed (CallFunction|CountWatchtowerTops))
      (Default|ShowTopRightQuestHUD _asspyro_player_controller "/Game/SpyroContent/CiC_Assets/CiC_Levels/Home_02_FutureRuins/00_FutureRuins/LevelItems/WatertowerTop/Eyeball_Flipbook_Mat.Eyeball_Flipbook_Mat" (Utilities|String|ToString(Integer) _total_number_destroyed) "6"))))

(fn ConstructionScript
  (|CallParentFunction))

(fn ShootFireball
  (bind _asspyro_persistant_data (Utilities|Casting|CastToSpyro_PersistantData (Game|GetGameInstance)))
  (if (Math|Boolean|ANDBoolean (not (Variables|/Game/SpyroContent/Global_Assets/Global_SaveData/Spyro_PersistantData.Spyro_PersistantData_C|GetPortal_Transition _asspyro_persistant_data)) (not (Variables|Default|GetContainer_Destroyed)) (not (Utilities|Enum|Equal(Enum) (Variables|Difficulty|GetMy%20Current%20Difficulty) "NewEnumerator0")))
    (for _array_element (Variables|Default|GetPlayers%20in%20My%20Range)
      (Utilities|IsValid _array_element
        (:Is%20Valid
          (Variables|/Game/SpyroContent/Global_Assets/Global_Characters/Playable_Characters/BP_Base_Playable.BP_Base_Playable_C|GetTalking_NPC _array_element
            (:then)
            (:else
              (bind _returnvalue (Game|SpawnActorfromClass "/Game/SpyroContent/Global_Assets/Global_Level_Items/Superflame/Superflame_BP.Superflame_BP_C" (Math|Transform|MakeTransform (+ (Transformation|GetWorldLocation (Variables|Default|GetCapsule%20Component)) (* (Math|Vector|GetForwardVector (Math|Rotator|FindLookatRotation (Transformation|GetWorldLocation (Variables|Default|GetCapsule%20Component)) (Transformation|GetActorLocation _array_element))) 1e+03)) (Math|Rotator|FindLookatRotation (Transformation|GetWorldLocation (Variables|Default|GetCapsule%20Component)) (Transformation|GetActorLocation _array_element)) "1,1,1") "AlwaysSpawn" 0 0))
              (Transformation|AddActorLocalRotation _returnvalue "0.000000,-89.800003,-1.500000" false false)
              (Variables|/Game/SpyroContent/Global_Assets/Global_Level_Items/Superflame/Superflame_BP.Superflame_BP_C|SetNo%20Creator _returnvalue true)
              (Audio|PlaySoundatLocation "/Game/SpyroContent/Global_Assets/Global_Level_Items/Superflame/Audio/Superflame.Superflame" (+ (Transformation|GetWorldLocation (Variables|Default|GetCapsule%20Component)) (* (Math|Vector|GetForwardVector (Math|Rotator|FindLookatRotation (Transformation|GetWorldLocation (Variables|Default|GetCapsule%20Component)) (Transformation|GetActorLocation _array_element))) 1e+03)) "0, 0, 0" 2.0 1.0 0.0 "/Game/SpyroContent/Global_Assets/Global_Audio/Attenuation/Spyro_Attenuation_Even_Farther.Spyro_Attenuation_Even_Farther" 0 0))))))))

(fn CountWatchtowerTops
  (LocalVariables|Setnumber%20destroyed 0)
  (bind _outactors (Actor|GetAllActorsOfClass "WatchtowerTop_BP_C"))
  (for _array_element _outactors
    (if (Variables|/Game/SpyroContent/Global_Assets/Global_Level_Items/Treasure_Containers/Treasure_Container_Base_BP.Treasure_Container_Base_BP_C|GetContainer_Destroyed _array_element)
      (Math|Integer|IncrementInt (LocalVariables|Getnumber%20destroyed))))
  (return (LocalVariables|Getnumber%20destroyed)))