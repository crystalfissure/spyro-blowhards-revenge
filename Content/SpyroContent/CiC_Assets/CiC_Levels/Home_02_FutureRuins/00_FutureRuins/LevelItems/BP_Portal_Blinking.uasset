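; Flickering level portal for Future Ruins that blinks on and off until the player overlaps it, then stays fully lit.
; A self-calling event loop toggles it at random short delays, starting on BeginPlay.
; Blink keeps surface visibility, audio, gold text and the normal or darker mesh material in sync.
; The parent's player overlap event sets a stop flag that forces everything on and ends the loop.
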(event Custom|Invoked%20Blink
  (if (not (Variables|Default|GetStop%20Blinking))
    (Utilities|FlowControl|Delay (Math|Random|RandomFloatinRange 0.4 2.0))
    (CallFunction|Blink)
    (CallFunction|InvokedBlink)))

(event Custom|Portal%20Overlapped
  (Variables|Default|SetStop%20Blinking true)
  (CallFunction|Blink))

(event EventBeginPlay
  (|CallParentFunction)
  (CallFunction|InvokedBlink)
  (EventDispatchers|BindEventtoPlayerOverlappedMe (delegate Custom|Portal%20Overlapped)))

(event EventTick
  (params (DeltaSeconds :type Float%20%28single-precision%29))
  (|CallParentFunction DeltaSeconds) ; This node is disabled and will not be called.\nDrag off pins to build functionality.
)

(fn ConstructionScript
  (|CallParentFunction))

(fn Blink
  (bind _portal_surface (Variables|Default|GetPortal_Surface))
  (bind _stop_blinking (Variables|Default|GetStop%20Blinking))
  (bind _bvisible (Variables|/Script/Engine.SceneComponent|GetbVisible _portal_surface))
  (bind _returnvalue (select _stop_blinking true _bvisible))
  (Rendering|SetVisibility _portal_surface (select (Variables|Default|GetStop%20Blinking) true (not _bvisible)) true)
  (Components|Activation|SetActive (Variables|Default|GetAudio) _returnvalue false)
  (Rendering|SetVisibility (Variables|Default|GetGold_Text_Actor) _returnvalue true)
  (Rendering|Material|SetMaterial (Variables|Default|GetStaticMesh) 0 (select (or _bvisible (Variables|Default|GetStop%20Blinking)) "/Game/SpyroContent/CiC_Assets/CiC_Levels/Home_02_FutureRuins/00_FutureRuins/Materials/Future_Ruins_2Sided.Future_Ruins_2Sided" "/Game/SpyroContent/CiC_Assets/CiC_Levels/Home_02_FutureRuins/00_FutureRuins/Materials/Future_Ruins_2Sided_Darker.Future_Ruins_2Sided_Darker")))