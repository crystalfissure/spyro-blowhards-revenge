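; WatchtowerBase_BP is a destructible treasure container in the Future Ruins level, serving as one of six watchtower quest objectives.
; It accepts only one damage type with super damage, then plays a blast effect and sound and spawns five shard bursts.
; It counts destroyed bases by scanning all instances, updating the quest HUD on destruction and reset.
; Successful damage also flags whether it was the last tower standing.
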(event Custom|Spawn%20Shards
  (bind _returnvalue (Math|Random|RandomFloatinRange -2e+01 2e+01))
  (bind _returnvalue_2 (Transformation|GetActorLocation))
  (bind _returnvalue_3 (Game|SpawnActorfromClass "/Game/SpyroContent/Global_Assets/Global_Level_Items/Treasure_Containers/Basket/Actors/Basket_Burst_BP.Basket_Burst_BP_C" (Math|Transform|MakeTransform (Math|Vector|MakeVector (+ (.x _returnvalue_2) _returnvalue) (+ (.y _returnvalue_2) _returnvalue) (+ (.z _returnvalue_2) _returnvalue)) "0, 0, 0" "1,1,1") "AlwaysSpawn" 0 0))
  (Default|ShardBurstAction _returnvalue_3 (Variables|Default|GetShard%20Mesh%201) (Variables|Default|GetShard%20Mesh%202)))

(event Custom|On%20Damage%20Dealt
  (bind _returnvalue (Transformation|GetActorLocation))
  (bind _damageable (Variables|Default|GetDamageable))
  (if (Math|Boolean|ANDBoolean (not (Variables|Default|GetContainer_Destroyed)) (Utilities|Enum|Equal(Enum) (Variables|/Game/SpyroContent/Global_Assets/Global_Components/Damageable_Com.Damageable_Com_C|GetDeal%20Damage%20-%20Damage%20Type _damageable) "NewEnumerator4") (Variables|/Game/SpyroContent/Global_Assets/Global_Components/Damageable_Com.Damageable_Com_C|GetDeal%20Damage%20-%20Super%20Damage _damageable))
    (Default|CallDamageWasSuccessfullyDealt (Variables|Default|GetDamageable))
    (Audio|PlaySoundatLocation "/Game/SpyroContent/Global_Assets/Global_Level_Items/Superflame/Audio/underwater_superflame_sound.underwater_superflame_sound" (Transformation|GetActorLocation) "0, 0, 0" 2.0 0.8 0.0 "/Game/SpyroContent/Global_Assets/Global_Audio/Attenuation/Spyro_Attenuation_Even_Farther.Spyro_Attenuation_Even_Farther" 0 0)
    (for _index (range 0 4)
      (CallFunction|SpawnShards))
    (Effects|SpawnEmitteratLocation "/Game/SpyroContent/Global_Assets/Global_Level_Items/Dragon_Breath/Blueprints/Aether/Particles/DarkAether_Blast.DarkAether_Blast" (Math|Vector|MakeVector (.x _returnvalue) (.y _returnvalue) (+ (.z _returnvalue) 1e+02)) "0, 0, 0" "5.000000,5.000000,5.000000")
    (bind _asspyro_player_controller (Utilities|Casting|CastToSpyro_PlayerController (Game|GetPlayerController 0)))
    (bind _total_number_destroyed (CallFunction|CountWatchtowerBases))
    (Default|ShowBottomRightQuestHUD _asspyro_player_controller "/Game/SpyroContent/CiC_Assets/CiC_Levels/Home_02_FutureRuins/00_FutureRuins/LevelItems/WatchtowerBase/Watchtower_Flipbook_Mat.Watchtower_Flipbook_Mat" (Utilities|String|ToString(Integer) _total_number_destroyed) "6")))

(event EventResetThisContainer
  (|CallParentFunction)
  (bind _asspyro_player_controller (Utilities|Casting|CastToSpyro_PlayerController (Game|GetPlayerController 0)))
  (bind _total_number_destroyed (CallFunction|CountWatchtowerBases))
  (Rendering|Components|TextRender|SetText (Variables|/Game/SpyroContent/Global_Assets/Global_UserInterface/Widgets/HUD.HUD_C|GetQuestItem_TextBlock_BottomRight (Variables|/Game/SpyroContent/Global_Assets/Global_Characters/Playable_Characters/Spyro_PlayerController.Spyro_PlayerController_C|GetMy_HUD_Ref _asspyro_player_controller)) (Utilities|Text|ToText(String) (Utilities|String|Append (Utilities|String|ToString(Integer) _total_number_destroyed) "/" "6"))))

(event EventBeginPlay
  (|CallParentFunction)
  (EventDispatchers|BindEventtoCallDealDamage (Variables|Default|GetDamageable) (delegate Custom|On%20Damage%20Dealt)))

(event EventTreasureContainerSuccessfullyDamaged
  (|CallParentFunction)
  (Variables|Default|SetIm_The_Last_Watchtower_Destroyed true)
  (bind _outactors (Actor|GetAllActorsOfClass "WatchtowerBase_BP_C"))
  (bind _array_element (Utilities|Array|ForEachLoopwithBreak _outactors)
    (:LoopBody
      (if (and (not (== _array_element self)) (not (Variables|/Game/SpyroContent/Global_Assets/Global_Level_Items/Treasure_Containers/Treasure_Container_Base_BP.Treasure_Container_Base_BP_C|GetContainer_Destroyed _array_element)))
        (Variables|Default|SetIm_The_Last_Watchtower_Destroyed false)))))

(fn ConstructionScript
  (|CallParentFunction))

(fn CountWatchtowerBases
  (LocalVariables|Setnumber%20destroyed 0)
  (bind _outactors (Actor|GetAllActorsOfClass "WatchtowerBase_BP_C"))
  (for _array_element _outactors
    (if (Variables|/Game/SpyroContent/Global_Assets/Global_Level_Items/Treasure_Containers/Treasure_Container_Base_BP.Treasure_Container_Base_BP_C|GetContainer_Destroyed _array_element)
      (Math|Integer|IncrementInt (LocalVariables|Getnumber%20destroyed))))
  (return (LocalVariables|Getnumber%20destroyed)))