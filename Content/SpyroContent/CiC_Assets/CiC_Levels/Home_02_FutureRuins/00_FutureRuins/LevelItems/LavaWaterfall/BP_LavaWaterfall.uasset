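; BP_LavaWaterfall is a lava waterfall hazard in the Future Ruins level that hurts the player and knocks them away on contact.
; When the waterfall component overlaps a playable character's capsule, it first checks that none of the three invincibility flags (damageable, cheat, super) is set.
; It then deals typed damage through the character's Damageable and launches them along its Arrow's forward vector, overriding their velocity.
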(event OnComponentBeginOverlap(FutureRuins_lava_waterfall)
  (params (OverlappedComponent :type Primitive%20Component%20Object%20Reference) (OtherActor :type Actor%20Object%20Reference) (OtherComp :type Primitive%20Component%20Object%20Reference) (OtherBodyIndex :type Integer) (bFromSweep :type Boolean) (SweepResult :type Hit%20Result%20Structure%20%28by%20ref%29))
  (bind _asbp_base_playable (Utilities|Casting|CastToBP_Base_Playable OtherActor))
  (if (Math|Boolean|ANDBoolean (== (Variables|/Script/Engine.Character|GetCapsuleComponent _asbp_base_playable) OtherComp) (not (Variables|/Game/SpyroContent/Global_Assets/Global_Components/Damageable_Com.Damageable_Com_C|GetInvincible (Variables|/Game/SpyroContent/Global_Assets/Global_Characters/Playable_Characters/BP_Base_Playable.BP_Base_Playable_C|GetDamageable _asbp_base_playable))) (not (Variables|/Game/SpyroContent/Global_Assets/Global_Characters/Playable_Characters/BP_Base_Playable.BP_Base_Playable_C|GetCHEAT_Invincibility _asbp_base_playable)) (not (Variables|/Game/SpyroContent/Global_Assets/Global_Characters/Playable_Characters/BP_Base_Playable.BP_Base_Playable_C|GetSuperinvincibility _asbp_base_playable)))
    (Default|DealDamage (Variables|/Game/SpyroContent/Global_Assets/Global_Characters/Playable_Characters/BP_Base_Playable.BP_Base_Playable_C|GetDamageable _asbp_base_playable) "NewEnumerator1" "0, 0, 0" false 0 false)
    (Character|LaunchCharacter _asbp_base_playable (* (Math|Vector|GetForwardVector (Variables|Default|GetArrow)) 2e+02) true true)))

(event EventBeginPlay)

(fn ConstructionScript)