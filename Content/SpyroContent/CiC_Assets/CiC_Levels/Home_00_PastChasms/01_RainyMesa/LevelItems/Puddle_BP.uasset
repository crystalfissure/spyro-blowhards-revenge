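; Puddle level item for Rainy Mesa that splashes and plays a footstep sound when the player steps onto it.
; While occupied, it binds to Spyro's anim Blueprint footstep event for further splashes, unbinding on step-off.
; Tick also splashes every frame while the player matches a specific environmental and player state.
; Splash spawns a forward-offset, lowered particle emitter plus a half-scale Water_Splash_BP actor at the player's location.
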(event Custom|On%20Spyro's%20Footstep
  (Variables|Default|GetPlayer%20on%20me
    (:then
      (CallFunction|Splash 4e+01))
    (:else)))

(event EventPlayerSteppedOntoMe
  (|CallParentFunction)
  (bind _player_on_me (Variables|Default|GetPlayer%20on%20me)
    (:then
      (CallFunction|Splash 0.0)
      (Audio|PlaySoundatLocation "/Game/SpyroContent/CiC_Assets/CiC_Levels/Home_00_PastChasms/01_RainyMesa/LevelItems/Audio/puddle_footstep_even.puddle_footstep_even" (Transformation|GetActorLocation _player_on_me) "0, 0, 0" 1.0 1.0 0.0 0 0 0)
      (bind _asabp_spyro (Utilities|Casting|CastToABP_Spyro (Components|SkeletalMesh|GetAnimInstance (Variables|/Script/Engine.Character|GetMesh _player_on_me))))
      (EventDispatchers|BindEventtoSpyroFootstep _asabp_spyro (delegate Custom|On%20Spyro's%20Footstep)))
    (:else)))

(event EventPlayerSteppedOffOfMe
  (|CallParentFunction)
  (bind _player_on_me (Variables|Default|GetPlayer%20on%20me)
    (:then
      (bind _asabp_spyro (Utilities|Casting|CastToABP_Spyro (Components|SkeletalMesh|GetAnimInstance (Variables|/Script/Engine.Character|GetMesh _player_on_me))))
      (EventDispatchers|UnbindEventfromSpyroFootstep _asabp_spyro (delegate Custom|On%20Spyro's%20Footstep)))
    (:else)))

(event EventTick
  (params (DeltaSeconds :type Float%20%28single-precision%29))
  (|CallParentFunction DeltaSeconds)
  (bind _player_on_me (Variables|Default|GetPlayer%20on%20me)
    (:then
      (if (and (Utilities|Enum|Equal(Enum) (Variables|/Game/SpyroContent/Global_Assets/Global_Characters/Playable_Characters/BP_Base_Playable.BP_Base_Playable_C|GetEnvironmental_State _player_on_me) "NewEnumerator0") (Utilities|Enum|Equal(Enum) (Variables|/Game/SpyroContent/Global_Assets/Global_Characters/Playable_Characters/BP_Base_Playable.BP_Base_Playable_C|GetPlayer_State _player_on_me) "NewEnumerator4"))
        (CallFunction|Splash 8e+01)))
    (:else)))

(event EventBeginPlay)

(fn ConstructionScript
  (|CallParentFunction))

(fn Splash
  (params (Forward%20Multiplier :type Float%20%28single-precision%29))
  (bind _player_on_me (Variables|Default|GetPlayer%20on%20me))
  (bind _returnvalue (Transformation|GetActorLocation _player_on_me))
  (bind _returnvalue_2 (Transformation|GetActorForwardVector _player_on_me))
  (bind _returnvalue_3 (* _returnvalue_2 Forward%20Multiplier))
  (bind _returnvalue_4 (+ _returnvalue _returnvalue_3))
  (Effects|SpawnEmitteratLocation "/Game/SpyroContent/Global_Assets/Global_Level_Items/Swimmable_Water/Particles/Splash_Particle.Splash_Particle" (Math|Vector|MakeVector (.x _returnvalue_4) (.y _returnvalue_4) (- (.z _returnvalue_4) 4e+01)))
  (Game|SpawnActorfromClass "/Game/SpyroContent/Global_Assets/Global_Level_Items/Swimmable_Water/Actors/Water_Splash_BP.Water_Splash_BP_C" (Math|Transform|MakeTransform _returnvalue "0, 0, 0" "0.500000,0.500000,0.500000") "AlwaysSpawn" 0 0))