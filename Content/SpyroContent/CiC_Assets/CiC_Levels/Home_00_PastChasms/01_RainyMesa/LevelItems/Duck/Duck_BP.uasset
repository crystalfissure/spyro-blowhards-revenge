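; Duck level item for the Rainy Mesa level that spawns and owns a companion puddle actor.
; On BeginPlay it spawns Duck_Puddle_BP slightly below itself, matching its mesh rotation and adding in the hit location of a zero-length WorldStatic trace.
; It copies its static mesh onto the puddle's Collision and Hitbox components.
; EndPlay destroys the puddle if it is still valid.
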(event EventBeginPlay
  (bind _returnvalue (Transformation|GetActorLocation))
  (bind _returnvalue_2 (Transformation|GetActorLocation))
  (bind _staticmesh (Variables|Default|GetStaticMesh))
  (bind _staticmesh_2 (Variables|/Script/Engine.StaticMeshComponent|GetStaticMesh _staticmesh))
  (|CallParentFunction)
  (bind _outhit (Collision|LineTraceForObjects _returnvalue _returnvalue (Utilities|Array|MakeArray "ObjectTypeQuery1") false 0 "None"))
  (bind _returnvalue_3 (Game|SpawnActorfromClass "/Game/SpyroContent/CiC_Assets/CiC_Levels/Home_00_PastChasms/01_RainyMesa/LevelItems/Duck/Duck_Puddle_BP.Duck_Puddle_BP_C" (Math|Transform|MakeTransform (Math|Vector|MakeVector (+ (.x _returnvalue_2) (.X (Math|Vector|BreakVector (.location _outhit)))) (+ (.y _returnvalue_2) (.Y (Math|Vector|BreakVector (.location _outhit)))) (+ (+ (.z _returnvalue_2) (.Z (Math|Vector|BreakVector (.location _outhit)))) -31.0)) (Transformation|GetWorldRotation (Variables|Default|GetStaticMesh)) "1,1,1") "AlwaysSpawn" 0 0))
  (Variables|Default|SetMy%20Puddle _returnvalue_3)
  (Components|StaticMesh|SetStaticMesh (Variables|/Game/SpyroContent/Global_Assets/Global_Level_Items/Wooden_Surface_BP.Wooden_Surface_BP_C|GetCollision _returnvalue_3) _staticmesh_2)
  (Components|StaticMesh|SetStaticMesh (Variables|/Game/SpyroContent/Global_Assets/Global_Level_Items/Wooden_Surface_BP.Wooden_Surface_BP_C|GetHitbox _returnvalue_3) _staticmesh_2))

(event EventEndPlay
  (params (EndPlayReason :type EEndPlayReason%20Enum :default "Destroyed"))
  (bind _my_puddle (Variables|Default|GetMy%20Puddle)
    (:then
      (Actor|DestroyActor _my_puddle))
    (:else)))

(fn ConstructionScript
  (|CallParentFunction))