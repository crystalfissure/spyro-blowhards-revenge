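; Fake reflection actor in the Rainy Mesa level that shows a mirrored copy of a playable character inside its box trigger.
; Overlap by the player's capsule unhides a skeletal mesh and feeds the player's mesh to its Spyro_PortalCopy_ABP as pose source.
; Each Tick the copy follows the player's XY, flips height about its starting Z and turns yaw 180 degrees.
; Only one player reflects at a time, until leaving the box.
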(event OnComponentBeginOverlap(Box)
  (params (OverlappedComponent :type Primitive%20Component%20Object%20Reference) (OtherActor :type Actor%20Object%20Reference) (OtherComp :type Primitive%20Component%20Object%20Reference) (OtherBodyIndex :type Integer) (bFromSweep :type Boolean) (SweepResult :type Hit%20Result%20Structure%20%28by%20ref%29))
  (bind _asbp_base_playable (Utilities|Casting|CastToBP_Base_Playable OtherActor))
  (if (== (Variables|/Script/Engine.Character|GetCapsuleComponent _asbp_base_playable) OtherComp)
    (Variables|Default|Getreflected%20player
      (:then)
      (:else
        (Variables|Default|Setreflected%20player _asbp_base_playable)
        (bind _asspyro_portal_copy_abp (Utilities|Casting|CastToSpyro_PortalCopy_ABP (Components|SkeletalMesh|GetAnimInstance (Variables|Default|GetSkeletalMesh))))
        (Variables|/Game/SpyroContent/Global_Assets/Global_Level_Items/Portals/Spyro_PortalCopy_ABP.Spyro_PortalCopy_ABP_C|SetSource%20Mesh%20Component _asspyro_portal_copy_abp (Variables|/Script/Engine.Character|GetMesh _asbp_base_playable))
        (Development|SetHiddeninGame (Variables|Default|GetSkeletalMesh) false false)))))

(event OnComponentEndOverlap(Box)
  (params (OverlappedComponent :type Primitive%20Component%20Object%20Reference) (OtherActor :type Actor%20Object%20Reference) (OtherComp :type Primitive%20Component%20Object%20Reference) (OtherBodyIndex :type Integer))
  (bind _asbp_base_playable (Utilities|Casting|CastToBP_Base_Playable OtherActor))
  (bind _reflected_player (Variables|Default|Getreflected%20player)
    (:then
      (if (and (== (Variables|/Script/Engine.Character|GetCapsuleComponent _asbp_base_playable) OtherComp) (== _reflected_player OtherActor))
        (Variables|Default|Setreflected%20player 0)
        (Development|SetHiddeninGame (Variables|Default|GetSkeletalMesh) true false)))
    (:else)))

(event EventBeginPlay
  (Variables|Default|SetStarting%20Z (.z (Transformation|GetWorldLocation (Variables|Default|GetSkeletalMesh)))))

(event EventTick
  (params (DeltaSeconds :type Float%20%28single-precision%29))
  (bind _reflected_player (Variables|Default|Getreflected%20player))
  (bind _mesh (Variables|/Script/Engine.Character|GetMesh _reflected_player))
  (bind _returnvalue (Transformation|GetWorldLocation _mesh))
  (bind _reflected_player_2 (Variables|Default|Getreflected%20player)
    (:then
      (Transformation|SetWorldRotation (Variables|Default|GetSkeletalMesh) (Math|Rotator|MakeRotator 0.0 0.0 (+ (.yaw (Transformation|GetWorldRotation (Variables|/Script/Engine.Character|GetMesh _reflected_player_2))) 1.8e+02)) false false)
      (Transformation|SetWorldLocation (Variables|Default|GetSkeletalMesh) (Math|Vector|MakeVector (.x _returnvalue) (.y _returnvalue) (- (Variables|Default|GetStarting%20Z) (- (.z _returnvalue) (Variables|Default|GetStarting%20Z)))) false false))
    (:else)))

(fn ConstructionScript)

(fn PlayerSteppedOntoMe)

(fn ReflectPlayer)