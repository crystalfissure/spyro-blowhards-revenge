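; Furnace vent hazard for the Rainy Mesa level that cycles between dormant, glowing warning and flame burst, with difficulty setting the dormant time.
; Timelines drive material color and fire scale; the hitbox grows during bursts, and overlap plus a looping box trace burn the player once per cycle.
; Certain damage types dampen the vent, flushing pending RetriggerableDelays with zero durations, then restarting the cycle after a short pause.
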(event OnComponentBeginOverlap(Hitbox)
  (params (OverlappedComponent :type Primitive%20Component%20Object%20Reference) (OtherActor :type Actor%20Object%20Reference) (OtherComp :type Primitive%20Component%20Object%20Reference) (OtherBodyIndex :type Integer) (bFromSweep :type Boolean) (SweepResult :type Hit%20Result%20Structure%20%28by%20ref%29))
  (if (and (>= (.z (Variables|/Script/Engine.SceneComponent|GetRelativeScale3D (Variables|Default|GetHitbox))) 1.0) (not (Variables|Default|GetVent%20is%20Damp)))
    (CallFunction|Damage? OtherActor OtherComp)))

(event Custom|Fire%20Vent%20Event
  (if (not (Variables|Default|GetVent%20is%20Damp))
    (Variables|Default|SetBurned%20Player false)
    (Utilities|FlowControl|Sequence
      (:then_0
        (bind _newtrack_0 (Timeline|Timeline_2 PlayFromStart)
          (:Update
            (Transformation|SetRelativeScale3D (Variables|Default|GetFire_Root) (Math|Vector|Lerp(Vector) (Variables|/Script/Engine.SceneComponent|GetRelativeScale3D (Variables|Default|GetFire_Root)) "0.010000,0.010000,0.010000" _newtrack_0)))))
      (:then_1
        (Rendering|Material|SetVectorParameterValue :self (Variables|Default|GetVent%20Mat%20Ref) :ParameterName "ColorChange" :!class /Script/Engine.MaterialInstanceDynamic)
        (Transformation|SetRelativeTransform (Variables|Default|GetHitbox) (Math|Transform|MakeTransform "0, 0,32.000000" "0, 0, 0" "1,1,0.150000") false false)
        (Components|Activation|Deactivate (Variables|Default|GetAudio))
        (Utilities|FlowControl|RetriggerableDelay (select (Variables|Default|GetVent%20is%20Damp) 0.0 (Utilities|Select :Index (Variables|Default|GetMy%20Current%20Difficulty) :NewEnumerator4 2.5 :NewEnumerator0 3.0 :NewEnumerator1 2.5 :NewEnumerator2 2.0 :NewEnumerator3 1.7)))
        (if (not (Variables|Default|GetVent%20is%20Damp))
          (Utilities|FlowControl|Sequence
            (:then_0
              (bind _newtrack_0_2 (Timeline|Timeline_0 PlayFromStart)
                (:Update
                  (Rendering|Material|SetVectorParameterValue (Variables|Default|GetVent%20Mat%20Ref) "ColorChange" (Math|Color|Lerp(LinearColor) :B "(R=1.000000,G=0.063954,B=0.000000,A=1.000000)" :Alpha _newtrack_0_2) :!class /Script/Engine.MaterialInstanceDynamic))))
            (:then_1
              (Utilities|FlowControl|RetriggerableDelay (select (Variables|Default|GetVent%20is%20Damp) 0.0 1.5))
              (if (not (Variables|Default|GetVent%20is%20Damp))
                (Utilities|FlowControl|Sequence
                  (:then_0
                    (bind _newtrack_0_3 (Timeline|Timeline_1 PlayFromStart)
                      (:Update
                        (Transformation|SetRelativeScale3D (Variables|Default|GetFire_Root) (Math|Vector|Lerp(Vector) "0.010000,0.010000,0.010000" "1.000000,1.000000,1.000000" _newtrack_0_3)))))
                  (:then_1
                    (Utilities|FlowControl|RetriggerableDelay (select (Variables|Default|GetVent%20is%20Damp) 0.0 0.2))
                    (if (not (Variables|Default|GetVent%20is%20Damp))
                      (Transformation|SetRelativeTransform (Variables|Default|GetHitbox) (Math|Transform|MakeTransform "0, 0,180.000000" "0, 0, 0" "1,1,1") false false)
                      (Components|Activation|Activate (Variables|Default|GetAudio) false)
                      (Audio|PlaySoundatLocation "/Game/SpyroContent/CiC_Assets/CiC_Level_Items/Dragon_Candle/Audio/light_fire.light_fire" (Transformation|GetActorLocation) "0, 0, 0" 1.0 1.0 0.0 "/Game/SpyroContent/Global_Assets/Global_Audio/Attenuation/Spyro_Attenuation_Farther.Spyro_Attenuation_Farther" 0 0)
                      (Utilities|FlowControl|RetriggerableDelay (select (Variables|Default|GetVent%20is%20Damp) 0.0 1.8))
                      (if (not (Variables|Default|GetVent%20is%20Damp))
                        (CallFunction|FireVentEvent)))))))))))))

(event Custom|Set%20My%20Difficulty
  (bind _asspyro_universal_save_data (CallFunction|LoadUniversalSave))
  (if (Utilities|Enum|Equal(Enum) (Variables|/Game/SpyroContent/Global_Assets/Global_SaveData/Spyro_Universal_Save_Data.Spyro_Universal_Save_Data_C|GetDifficulty _asspyro_universal_save_data) "NewEnumerator4")
    (bind _asspyro_save_data (CallFunction|LoadSpyroGame self))
    (bind _difficulty (CallFunction|ConvertSkillLevelFloattoEnum (Variables|/Game/SpyroContent/Global_Assets/Global_SaveData/Spyro_SaveData.Spyro_SaveData_C|GetSkill_Level _asspyro_save_data)))
    (Variables|Default|SetMy%20Current%20Difficulty _difficulty)
    (else
      (Variables|Default|SetMy%20Current%20Difficulty (Variables|/Game/SpyroContent/Global_Assets/Global_SaveData/Spyro_Universal_Save_Data.Spyro_Universal_Save_Data_C|GetDifficulty _asspyro_universal_save_data)))))

(event Custom|Dampen%20Vent
  (|CollapseGraph_0)
  (Variables|Default|SetVent%20is%20Damp true)
  (Utilities|FlowControl|Sequence
    (:then_0
      (bind _newtrack_0 (Timeline|Timeline_2 Stop)
        (:Update
          (Transformation|SetRelativeScale3D (Variables|Default|GetFire_Root) (Math|Vector|Lerp(Vector) (Variables|/Script/Engine.SceneComponent|GetRelativeScale3D (Variables|Default|GetFire_Root)) "0.010000,0.010000,0.010000" _newtrack_0)))))
    (:then_1
      (Utilities|FlowControl|RetriggerableDelay (select (Variables|Default|GetVent%20is%20Damp) 0.0 (Utilities|Select :Index (Variables|Default|GetMy%20Current%20Difficulty) :NewEnumerator4 2.5 :NewEnumerator0 3.0 :NewEnumerator1 2.5 :NewEnumerator2 2.0 :NewEnumerator3 1.7)))
      (if (not (Variables|Default|GetVent%20is%20Damp))
        (Utilities|FlowControl|Sequence
          (:then_0
            (bind _newtrack_0_2 (Timeline|Timeline_0 PlayFromStart)
              (:Update
                (Rendering|Material|SetVectorParameterValue (Variables|Default|GetVent%20Mat%20Ref) "ColorChange" (Math|Color|Lerp(LinearColor) :B "(R=1.000000,G=0.063954,B=0.000000,A=1.000000)" :Alpha _newtrack_0_2) :!class /Script/Engine.MaterialInstanceDynamic))))
          (:then_1
            (Utilities|FlowControl|RetriggerableDelay (select (Variables|Default|GetVent%20is%20Damp) 0.0 1.5) :!label _label)
            (if (not (Variables|Default|GetVent%20is%20Damp))
              (Utilities|FlowControl|Sequence
                (:then_0
                  (bind _newtrack_0_3 (Timeline|Timeline_1 PlayFromStart)
                    (:Update
                      (Transformation|SetRelativeScale3D (Variables|Default|GetFire_Root) (Math|Vector|Lerp(Vector) "0.010000,0.010000,0.010000" "1.000000,1.000000,1.000000" _newtrack_0_3)))))
                (:then_1
                  (Utilities|FlowControl|RetriggerableDelay (select (Variables|Default|GetVent%20is%20Damp) 0.0 0.2) :!label _label_2)
                  (if (not (Variables|Default|GetVent%20is%20Damp))
                    (Transformation|SetRelativeTransform (Variables|Default|GetHitbox) (Math|Transform|MakeTransform "0, 0,180.000000" "0, 0, 0" "1,1,1") false false)
                    (Components|Activation|Activate (Variables|Default|GetAudio) false)
                    (Audio|PlaySoundatLocation "/Game/SpyroContent/CiC_Assets/CiC_Level_Items/Dragon_Candle/Audio/light_fire.light_fire" (Transformation|GetActorLocation) "0, 0, 0" 1.0 1.0 0.0 "/Game/SpyroContent/Global_Assets/Global_Audio/Attenuation/Spyro_Attenuation_Farther.Spyro_Attenuation_Farther" 0 0)
                    (Utilities|FlowControl|RetriggerableDelay (select (Variables|Default|GetVent%20is%20Damp) 0.0 1.8) :!label _label_3)
                    (if (not (Variables|Default|GetVent%20is%20Damp))
                      (CallFunction|FireVentEvent))))))))))
    (:then_2
      (Timeline|Timeline_0 Stop))
    (:then_3
      (goto _label))
    (:then_4
      (Timeline|Timeline_1 Stop))
    (:then_5
      (goto _label_3))
    (:then_6
      (goto _label_2))
    (:then_7
      (Rendering|Material|SetVectorParameterValue :self (Variables|Default|GetVent%20Mat%20Ref) :ParameterName "ColorChange" :!class /Script/Engine.MaterialInstanceDynamic)
      (Transformation|SetRelativeTransform (Variables|Default|GetHitbox) (Math|Transform|MakeTransform "0, 0,32.000000" "0, 0, 0" "1,1,0.150000") false false)
      (Components|Activation|Deactivate (Variables|Default|GetAudio))
      (bind _newtrack_0_4 (Timeline|Timeline_3 PlayFromStart)
        (:Update
          (Transformation|SetRelativeScale3D (Variables|Default|GetFire_Root) (Math|Vector|Lerp(Vector) (Variables|/Script/Engine.SceneComponent|GetRelativeScale3D (Variables|Default|GetFire_Root)) "0.010000,0.010000,0.010000" _newtrack_0_4)))))
    (:then_8
      (Utilities|FlowControl|RetriggerableDelay 1.0)
      (Variables|Default|SetVent%20is%20Damp false)
      (CallFunction|FireVentEvent))))

(event Custom|On%20Vent%20Damaged
  (bind _damageable_comp (Variables|Default|GetDamageable_Comp))
  (bind _deal_damage___damage_type (Variables|/Game/SpyroContent/Global_Assets/Global_Components/Damageable_Com.Damageable_Com_C|GetDeal%20Damage%20-%20Damage%20Type _damageable_comp))
  (if (Math|Boolean|ORBoolean (Utilities|Enum|Equal(Enum) _deal_damage___damage_type "NewEnumerator7") (Utilities|Enum|Equal(Enum) _deal_damage___damage_type "NewEnumerator9") (Utilities|Enum|Equal(Enum) _deal_damage___damage_type "NewEnumerator10") (Utilities|Enum|Equal(Enum) _deal_damage___damage_type "NewEnumerator11") (Utilities|Enum|Equal(Enum) _deal_damage___damage_type "NewEnumerator12") (Utilities|Enum|Equal(Enum) _deal_damage___damage_type "NewEnumerator13"))
    (CallFunction|DampenVent)))

(event EventBeginPlay
  (bind _furnace_vent (Variables|Default|Getfurnace_vent))
  (bind _returnvalue (Rendering|Material|CreateDynamicMaterialInstance _furnace_vent 1 (Rendering|Material|GetMaterial _furnace_vent 1) "None" :!class /Script/Engine.PrimitiveComponent))
  (Variables|Default|SetVent%20Mat%20Ref _returnvalue)
  (CallFunction|FireVentEvent)
  (Variables|/Game/SpyroContent/Global_Assets/Global_Components/Damageable_Com.Damageable_Com_C|SetObject's%20Hitbox%20Component (Variables|Default|GetDamageable_Comp) (Variables|Default|GetHitbox))
  (EventDispatchers|BindEventtoCallDealDamage (Variables|Default|GetDamageable_Comp) (delegate Custom|On%20Vent%20Damaged))
  (Utilities|Time|SetTimerbyFunctionName 0 "Burn Ping" 0.2 true)
  (bind _asspyro_persistant_data (Utilities|Casting|CastToSpyro_PersistantData (Game|GetGameInstance))
    (:then
      (EventDispatchers|BindEventtoDifficultyChanged _asspyro_persistant_data (delegate Custom|Set%20My%20Difficulty)))
    (:CastFailed
      _))
  (CallFunction|SetMyDifficulty))

(fn ConstructionScript)

(fn BurnPing
  (bind _returnvalue (Transformation|GetActorLocation))
  (if (and (>= (.z (Variables|/Script/Engine.SceneComponent|GetRelativeScale3D (Variables|Default|GetHitbox))) 1.0) (not (Variables|Default|GetVent%20is%20Damp)))
    (bind _outhits (Class|KismetSystemLibrary|BoxTraceMultiforObjects _returnvalue _returnvalue "160.000000,160.000000,160.000000" "0, 0, 0" (Utilities|Array|MakeArray "ObjectTypeQuery3" "ObjectTypeQuery9" "ObjectTypeQuery10" "ObjectTypeQuery8") false 0 "None" true))
    (for _array_element _outhits
      (CallFunction|Damage? (.hitactor _array_element) (.hitcomponent _array_element)))))

(fn Damage?
  (params (Actor :type Object%20Object%20Reference) (Comp :type Object%20Object%20Reference))
  (bind _asbp_base_playable (Utilities|Casting|CastToBP_Base_Playable Actor))
  (if (Math|Boolean|ANDBoolean (== (Variables|/Script/Engine.Character|GetCapsuleComponent _asbp_base_playable) Comp) (not (Variables|Default|GetBurned%20Player)) (not (Utilities|Enum|Equal(Enum) (Variables|/Game/SpyroContent/Global_Assets/Global_Characters/Playable_Characters/BP_Base_Playable.BP_Base_Playable_C|GetPlayer_State _asbp_base_playable) "NewEnumerator19")))
    (Default|DealDamage (Variables|/Game/SpyroContent/Global_Assets/Global_Characters/Playable_Characters/BP_Base_Playable.BP_Base_Playable_C|GetDamageable _asbp_base_playable) "NewEnumerator1" "0, 0, 0" false 0 false)
    (Variables|Default|SetBurned%20Player true)))