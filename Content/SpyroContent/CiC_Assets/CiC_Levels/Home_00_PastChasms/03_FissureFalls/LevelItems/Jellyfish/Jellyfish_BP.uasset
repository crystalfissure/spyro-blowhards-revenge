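; Jellyfish enemy for the Fissure Falls level that electrifies its referenced water while alerted.
; State changes from its WalkingAICharacter set gravity, which is on only when dying, and start or reset the shock cycle.
; While Alert, a retriggerable delay loops the shock at a difficulty-scaled interval; other states collapse the delay to zero, and the state check ends the loop.
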(event Custom|on%20jellyfish%20state%20changed
  (Variables|/Script/Engine.CharacterMovementComponent|SetGravityScale (Variables|Character|GetCharacterMovement) (select (Utilities|Enum|Equal(Enum) (Variables|/Game/SpyroContent/Global_Assets/Global_Components/Base_AI_Character.Base_AI_Character_C|GetAICharacter_State (Variables|Default|GetWalking_AI_Character)) "NewEnumerator3") 1.0 0.0))
  (switch Utilities|FlowControl|Switch|SwitchonAICharacter_States (Variables|/Game/SpyroContent/Global_Assets/Global_Components/Base_AI_Character.Base_AI_Character_C|GetAICharacter_State (Variables|Default|GetWalking_AI_Character))
    (:NewEnumerator0
      (CallFunction|UnalertedJelly :!label _label))
    (:NewEnumerator1
      (CallFunction|ShocktheWater))
    (:NewEnumerator2
      (goto _label))
    (:NewEnumerator3
      (goto _label))))

(event Custom|shock%20the%20water
  (bind _medium_time (Variables|Default|GetMedium%20time))
  (switch Utilities|FlowControl|Switch|SwitchonAICharacter_States (Variables|/Game/SpyroContent/Global_Assets/Global_Components/Base_AI_Character.Base_AI_Character_C|GetAICharacter_State (Variables|Default|GetWalking_AI_Character))
    (:NewEnumerator1
      (bind _water_ref (Variables|Default|GetWater%20Ref)
        (:then
          (Default|ElectrifyWater _water_ref)
          (Utilities|FlowControl|RetriggerableDelay (select (Utilities|Enum|Equal(Enum) (Variables|/Game/SpyroContent/Global_Assets/Global_Components/Base_AI_Character.Base_AI_Character_C|GetAICharacter_State (Variables|Default|GetWalking_AI_Character)) "NewEnumerator1") (+ 3.0 (Utilities|Select :Index (Variables|Default|GetMy%20Current%20Difficulty) :NewEnumerator4 _medium_time :NewEnumerator0 (Variables|Default|GetEasy%20time) :NewEnumerator1 _medium_time :NewEnumerator2 (Variables|Default|Gethard%20time) :NewEnumerator3 (Variables|Default|GetNightmare%20time))) 0.0))
          (CallFunction|ShocktheWater))
        (:else)))))

(event Custom|unalerted%20jelly
  (bind _medium_time (Variables|Default|GetMedium%20time))
  (Utilities|FlowControl|RetriggerableDelay (select (Utilities|Enum|Equal(Enum) (Variables|/Game/SpyroContent/Global_Assets/Global_Components/Base_AI_Character.Base_AI_Character_C|GetAICharacter_State (Variables|Default|GetWalking_AI_Character)) "NewEnumerator1") (+ 3.0 (Utilities|Select :Index (Variables|Default|GetMy%20Current%20Difficulty) :NewEnumerator4 _medium_time :NewEnumerator0 (Variables|Default|GetEasy%20time) :NewEnumerator1 _medium_time :NewEnumerator2 (Variables|Default|Gethard%20time) :NewEnumerator3 (Variables|Default|GetNightmare%20time))) 0.0))
  (CallFunction|ShocktheWater))

(event EventBeginPlay
  (|CallParentFunction)
  (EventDispatchers|BindEventtoMyStateChanged (Variables|Default|GetWalking_AI_Character) (delegate Custom|on%20jellyfish%20state%20changed)))

(fn ConstructionScript
  (|CallParentFunction))