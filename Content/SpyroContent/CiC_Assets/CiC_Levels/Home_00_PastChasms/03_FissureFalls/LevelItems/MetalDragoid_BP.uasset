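; MetalDragoid_BP is a metal Dragoid AI character in the Fissure Falls level that shatters like a metal crate when it dies.
; On BeginPlay it registers its mesh as the Damageable component's metal-material component and listens for AI state changes.
; Entering the Dying state spawns a Basket_Burst_BP slightly below the actor, bursts it with metal chest shard meshes and plays a crate-break sound.
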(event Custom|On%20State%20Change
  (bind _returnvalue (Transformation|GetActorTransform))
  (switch Utilities|FlowControl|Switch|SwitchonAICharacter_States (Variables|/Game/SpyroContent/Global_Assets/Global_Components/Base_AI_Character.Base_AI_Character_C|GetAICharacter_State (Variables|Default|GetWalking_AI_Character))
    (:NewEnumerator3
      (bind _returnvalue_2 (Game|SpawnActorfromClass "/Game/SpyroContent/Global_Assets/Global_Level_Items/Treasure_Containers/Basket/Actors/Basket_Burst_BP.Basket_Burst_BP_C" (Math|Transform|MakeTransform (Math|Vector|MakeVector (.x (.location _returnvalue)) (.y (.location _returnvalue)) (- (.z (.location _returnvalue)) 1e+02)) (.rotation _returnvalue) (.scale _returnvalue)) "AlwaysSpawn" 0 0))
      (Default|ShardBurstAction _returnvalue_2 "/Game/SpyroContent/Global_Assets/Global_Level_Items/Treasure_Containers/Metal_Chest/Meshes/metal_chest_shard.metal_chest_shard" "/Game/SpyroContent/Global_Assets/Global_Level_Items/Treasure_Containers/Metal_Chest/Meshes/metal_chest_shard_2.metal_chest_shard_2")
      (Audio|PlaySoundatLocation "/Game/SpyroContent/Global_Assets/Global_Level_Items/Treasure_Containers/Metal_Chest/MetalCrateBreak1.MetalCrateBreak1" (Transformation|GetActorLocation) "0, 0, 0" 1.0 1.0 0.0 0 0 0))))

(event EventBeginPlay
  (|CallParentFunction)
  (Variables|/Game/SpyroContent/Global_Assets/Global_Components/Damageable_Com.Damageable_Com_C|SetComponent_with_Metal_Material (Variables|Default|GetDamageable) (Variables|Character|GetMesh))
  (EventDispatchers|BindEventtoMyStateChanged (Variables|Default|GetWalking_AI_Character) (delegate Custom|On%20State%20Change)))

(event Collision|EventActorBeginOverlap
  (params (OtherActor :type Actor%20Object%20Reference)))

(event EventTick
  (params (DeltaSeconds :type Float%20%28single-precision%29))
  (|CallParentFunction DeltaSeconds) ; This node is disabled and will not be called.\nDrag off pins to build functionality.
)

(fn ConstructionScript
  (|CallParentFunction))