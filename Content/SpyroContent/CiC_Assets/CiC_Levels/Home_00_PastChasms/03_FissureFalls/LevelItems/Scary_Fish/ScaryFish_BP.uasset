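; Scary fish enemy for the Fissure Falls level, driven by the WalkingAICharacter state machine.
; Idle eases it back to its spawn point; Attacking plays a sound and, while on camera, lunges with difficulty-scaled impulses while facing the player.
; Dying sets gravity scale to normal.
; Chomp box-traces for Damageable hitboxes and deals super damage while attacking; the older capsule-hit damage logic is disconnected.
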(event OnComponentHit(CapsuleComponent)
  (params (HitComponent :type Primitive%20Component%20Object%20Reference) (OtherActor :type Actor%20Object%20Reference) (OtherComp :type Primitive%20Component%20Object%20Reference) (NormalImpulse :type Vector :default "0, 0, 0") (Hit :type Hit%20Result%20Structure%20%28by%20ref%29)))

(event Custom|on%20state%20change
  (switch Utilities|FlowControl|Switch|SwitchonAICharacter_States (Variables|/Game/SpyroContent/Global_Assets/Global_Components/Base_AI_Character.Base_AI_Character_C|GetAICharacter_State (Variables|Default|GetWalking_AI_Character))
    (:NewEnumerator2
      (Audio|PlaySoundatLocation "/Game/SpyroContent/CiC_Assets/CiC_Levels/Home_00_PastChasms/03_FissureFalls/LevelItems/Scary_Fish/scary_fish_sfx.scary_fish_sfx" (Transformation|GetActorLocation) "0, 0, 0" 1.0 1.0 0.0 0 0 0))
    (:NewEnumerator3
      (Variables|/Script/Engine.CharacterMovementComponent|SetGravityScale (Variables|Character|GetCharacterMovement) 1.0))))

(event EventBeginPlay
  (|CallParentFunction)
  (EventDispatchers|BindEventtoMyStateChanged (Variables|Default|GetWalking_AI_Character) (delegate Custom|on%20state%20change)))

(event EventTick
  (params (DeltaSeconds :type Float%20%28single-precision%29))
  (switch Utilities|FlowControl|Switch|SwitchonAICharacter_States (Variables|/Game/SpyroContent/Global_Assets/Global_Components/Base_AI_Character.Base_AI_Character_C|GetAICharacter_State (Variables|Default|GetWalking_AI_Character))
    (:NewEnumerator0
      (if (not (Math|Vector|Equal(Vector) (Transformation|GetActorLocation) (Variables|/Game/SpyroContent/Global_Assets/Global_Components/Base_AI_Character.Base_AI_Character_C|GetSpawn_Point (Variables|Default|GetWalking_AI_Character)) 0.1))
        (Transformation|SetActorLocation (Math|Vector|Lerp(Vector) (Transformation|GetActorLocation) (Variables|/Game/SpyroContent/Global_Assets/Global_Components/Base_AI_Character.Base_AI_Character_C|GetSpawn_Point (Variables|Default|GetWalking_AI_Character)) (* (Utilities|Time|GetWorldDeltaSeconds) 1.0)) false false)))
    (:NewEnumerator2
      (bind _returnvalue (CallFunction|AmIonCamera?))
      (if _returnvalue
        (Physics|AddImpulse (Variables|Character|GetCharacterMovement) (* (Transformation|GetActorForwardVector) (Utilities|Select :Index (Variables|Default|GetMy%20Current%20Difficulty) :NewEnumerator4 75.0 :NewEnumerator0 5e+01 :NewEnumerator1 75.0 :NewEnumerator2 1e+02 :NewEnumerator3 1.1e+02)) false)
        (Default|LookatPlayer (Variables|Default|GetWalking_AI_Character))))))

(fn ConstructionScript
  (|CallParentFunction))

(fn Chomp
  (bind _box (Variables|Default|GetBox))
  (bind _returnvalue (Transformation|GetWorldLocation _box))
  (bind _outhits (Class|KismetSystemLibrary|BoxTraceMultiforObjects _returnvalue _returnvalue "75.000000,125.000000,75.000000" (Transformation|GetWorldRotation _box) (Utilities|Array|MakeArray "ObjectTypeQuery3" "ObjectTypeQuery9" "ObjectTypeQuery8" "ObjectTypeQuery10") false 0 "None" true))
  (for _array_element _outhits
    (Utilities|IsValid (Actor|GetComponentbyClass (.hitactor _array_element) "/Game/SpyroContent/Global_Assets/Global_Components/Damageable_Com.Damageable_Com_C")
      (:Is%20Valid
        (if (and (== (Variables|/Game/SpyroContent/Global_Assets/Global_Components/Damageable_Com.Damageable_Com_C|GetObject's%20Hitbox%20Component (Actor|GetComponentbyClass (.hitactor _array_element) "/Game/SpyroContent/Global_Assets/Global_Components/Damageable_Com.Damageable_Com_C")) (.hitcomponent _array_element)) (Utilities|Enum|Equal(Enum) (Variables|/Game/SpyroContent/Global_Assets/Global_Components/Base_AI_Character.Base_AI_Character_C|GetAICharacter_State (Variables|Default|GetWalking_AI_Character)) "NewEnumerator2"))
          (Default|DealDamage (Actor|GetComponentbyClass (.hitactor _array_element) "/Game/SpyroContent/Global_Assets/Global_Components/Damageable_Com.Damageable_Com_C") "NewEnumerator0" (Transformation|GetActorForwardVector) true self false))))))