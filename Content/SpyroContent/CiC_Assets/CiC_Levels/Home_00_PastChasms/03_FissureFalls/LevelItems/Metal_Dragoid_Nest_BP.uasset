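; Metal Dragoid Nest is a damageable treasure container used as a level item in Fissure Falls.
; On BeginPlay it registers its static mesh as the Damageable component's metal-material component.
; It ignores successful damage dealt by Dragoids and passes all other hits, including those with no valid dealer, to the parent's damage handling.
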(event EventBeginPlay
  (|CallParentFunction)
  (Variables|/Game/SpyroContent/Global_Assets/Global_Components/Damageable_Com.Damageable_Com_C|SetComponent_with_Metal_Material (Variables|Default|GetDamageable) (Variables|Default|GetStaticMesh)))

(event EventTreasureContainerSuccessfullyDamaged
  (bind _deal_damage___person_who_dealt_the_damage (Variables|/Game/SpyroContent/Global_Assets/Global_Components/Damageable_Com.Damageable_Com_C|GetDeal%20Damage%20-%20Person%20Who%20Dealt%20the%20Damage (Variables|Default|GetDamageable))
    (:then
      (Utilities|Casting|CastToDragoid_BP _deal_damage___person_who_dealt_the_damage
        (:CastFailed
          _)))
    (:else
      _))
  (|CallParentFunction))

(fn ConstructionScript
  (|CallParentFunction))