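; Fissure Falls Draklet enemy that hangs at its spawn point and drops, with a slide whistle, when the player enters its drop box.
; Its capsule overlaps to deal super damage while moving, then switches to blocking on landing.
; After a delay, a timeline lerps it back up while pinning its drop shadow, then a box trace re-checks for players below.
; One AI state restores gravity and suspends this cycle.
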(event OnComponentBeginOverlap(Drop_Box)
  (params (OverlappedComponent :type Primitive%20Component%20Object%20Reference) (OtherActor :type Actor%20Object%20Reference) (OtherComp :type Primitive%20Component%20Object%20Reference) (OtherBodyIndex :type Integer) (bFromSweep :type Boolean) (SweepResult :type Hit%20Result%20Structure%20%28by%20ref%29))
  (CallFunction|DropBoxOverlapCheck OtherActor OtherComp))

(event OnComponentBeginOverlap(CapsuleComponent)
  (params (OverlappedComponent :type Primitive%20Component%20Object%20Reference) (OtherActor :type Actor%20Object%20Reference) (OtherComp :type Primitive%20Component%20Object%20Reference) (OtherBodyIndex :type Integer) (bFromSweep :type Boolean) (SweepResult :type Hit%20Result%20Structure%20%28by%20ref%29))
  (bind _asbp_base_playable (Utilities|Casting|CastToBP_Base_Playable OtherActor))
  (if (Math|Boolean|ANDBoolean (== (Variables|/Script/Engine.Character|GetCapsuleComponent _asbp_base_playable) OtherComp) (not (Utilities|Enum|Equal(Enum) (Variables|/Game/SpyroContent/Global_Assets/Global_Characters/Playable_Characters/BP_Base_Playable.BP_Base_Playable_C|GetPlayer_State _asbp_base_playable) "NewEnumerator11")) (not (Utilities|Enum|Equal(Enum) (Variables|/Game/SpyroContent/Global_Assets/Global_Characters/Playable_Characters/BP_Base_Playable.BP_Base_Playable_C|GetPlayer_State _asbp_base_playable) "NewEnumerator4")) (not (Utilities|Enum|Equal(Enum) (Variables|/Game/SpyroContent/Global_Assets/Global_Characters/Playable_Characters/BP_Base_Playable.BP_Base_Playable_C|GetPlayer_State _asbp_base_playable) "NewEnumerator8")) (> (Math|Vector|VectorLength (Transformation|GetVelocity)) 1e+01) (not (Utilities|Enum|Equal(Enum) (Variables|/Game/SpyroContent/Global_Assets/Global_Components/Base_AI_Character.Base_AI_Character_C|GetAICharacter_State (Variables|Default|GetWalking_AI_Character)) "NewEnumerator3")))
    (Default|DealDamage (Variables|/Game/SpyroContent/Global_Assets/Global_Characters/Playable_Characters/BP_Base_Playable.BP_Base_Playable_C|GetDamageable _asbp_base_playable) "NewEnumerator4" (Transformation|GetActorForwardVector) true self false)))

(event Custom|on%20draklet%20state%20changed
  (bind _walking_ai_character (Variables|Default|GetWalking_AI_Character))
  (bind _aicharacter_state (Variables|/Game/SpyroContent/Global_Assets/Global_Components/Base_AI_Character.Base_AI_Character_C|GetAICharacter_State _walking_ai_character))
  (bind _returnvalue (Utilities|Enum|Equal(Enum) _aicharacter_state "NewEnumerator3"))
  (Variables|/Script/Engine.CharacterMovementComponent|SetGravityScale (Variables|Character|GetCharacterMovement) (select _returnvalue 1.0 0.0))
  (if _returnvalue
    (CallFunction|StopGoingBackUp))
  (if (Utilities|Enum|Equal(Enum) (Variables|/Game/SpyroContent/Global_Assets/Global_Components/Base_AI_Character.Base_AI_Character_C|GetPrevious%20AI%20State (Variables|Default|GetWalking_AI_Character)) "NewEnumerator3")
    (CallFunction|UnblockCapsuleCOL)))

(event Custom|go%20back%20up
  (bind _damageable (Variables|Default|GetDamageable))
  (Utilities|FlowControl|Delay 1.5)
  (if (not (Utilities|Enum|Equal(Enum) (Variables|/Game/SpyroContent/Global_Assets/Global_Components/Base_AI_Character.Base_AI_Character_C|GetAICharacter_State (Variables|Default|GetWalking_AI_Character)) "NewEnumerator3"))
    (if (and (not (Variables|/Game/SpyroContent/Global_Assets/Global_Components/Damageable_Com.Damageable_Com_C|GetFrozen _damageable)) (not (Variables|/Game/SpyroContent/Global_Assets/Global_Components/Damageable_Com.Damageable_Com_C|GetParalyzed_by_Fear _damageable)))
      (Audio|PlaySoundatLocation "/Game/SpyroContent/CiC_Assets/CiC_Levels/Home_00_PastChasms/03_FissureFalls/LevelItems/Drop_Draklet/slide_whistle_up.slide_whistle_up" (Transformation|GetWorldLocation (Variables|Default|GetCapsuleComponent)) "0, 0, 0" 1.0 1.0 0.0 0 0 0))
    (CallFunction|UnblockCapsuleCOL)
    (Variables|/Script/Engine.CharacterMovementComponent|SetGravityScale (Variables|Character|GetCharacterMovement) 0.0)
    (Variables|Default|Setgoing%20back%20up true)
    (bind _newtrack_0 (Timeline|Timeline_1 PlayFromStart)
      (:Update
        (Transformation|SetActorLocation (Math|Vector|Lerp(Vector) (Transformation|GetActorLocation) (Variables|/Game/SpyroContent/Global_Assets/Global_Components/Base_AI_Character.Base_AI_Character_C|GetSpawn_Point (Variables|Default|GetWalking_AI_Character)) _newtrack_0) false false)
        (Transformation|SetWorldLocation (Variables|Default|GetAIs_DropShadow) (Variables|Default|Getdrop%20shadow%20location) false false))
      (:Finished
        (Variables|Default|Setgoing%20back%20up false)
        (CallFunction|DropBoxPing)))))

(event Custom|stop%20going%20back%20up
  (Variables|Default|Setgoing%20back%20up false)
  (CallFunction|DropBoxPing)
  (bind _newtrack_0 (Timeline|Timeline_1 Stop)
    (:Update
      (Transformation|SetActorLocation (Math|Vector|Lerp(Vector) (Transformation|GetActorLocation) (Variables|/Game/SpyroContent/Global_Assets/Global_Components/Base_AI_Character.Base_AI_Character_C|GetSpawn_Point (Variables|Default|GetWalking_AI_Character)) _newtrack_0) false false)
      (Transformation|SetWorldLocation (Variables|Default|GetAIs_DropShadow) (Variables|Default|Getdrop%20shadow%20location) false false))
    (:Finished
      (Variables|Default|Setgoing%20back%20up false)
      (CallFunction|DropBoxPing))))

(event EventBeginPlay
  (|CallParentFunction)
  (EventDispatchers|BindEventtoMyStateChanged (Variables|Default|GetWalking_AI_Character) (delegate Custom|on%20draklet%20state%20changed))
  (CallFunction|UnblockCapsuleCOL)
  (Utilities|FlowControl|Delay 0.2)
  (Variables|Default|Setdrop%20shadow%20location (Transformation|GetWorldLocation (Variables|Default|GetAIs_DropShadow))))

(event EventOnMovementModeChanged
  (params (PrevMovementMode :type EMovementMode%20Enum :default "MOVE_None") (NewMovementMode :type EMovementMode%20Enum :default "MOVE_None") (PrevCustomMode :type Byte :default 0) (NewCustomMode :type Byte :default 0))
  (if (and (Utilities|Enum|Equal(Enum) PrevMovementMode "MOVE_Falling") (Utilities|Enum|Equal(Enum) NewMovementMode "MOVE_Walking"))
    (CallFunction|BlockCapsuleCOL))
  (|CallParentFunction PrevMovementMode NewMovementMode PrevCustomMode NewCustomMode))

(event EventResetThisAICharacter
  (|CallParentFunction)
  (CallFunction|UnblockCapsuleCOL))

(fn ConstructionScript
  (|CallParentFunction))

(fn UnblockCapsuleCOL
  (bind _capsulecomponent (Variables|Default|GetCapsuleComponent))
  (if (not (Utilities|Enum|Equal(Enum) (Variables|/Game/SpyroContent/Global_Assets/Global_Components/Base_AI_Character.Base_AI_Character_C|GetAICharacter_State (Variables|Default|GetWalking_AI_Character)) "NewEnumerator3"))
    (Collision|SetCollisionResponsetoChannel _capsulecomponent "ECC_Pawn" "ECR_Overlap")
    (Collision|SetCollisionResponsetoChannel _capsulecomponent "ECC_GameTraceChannel4" "ECR_Overlap")
    (Collision|SetCollisionResponsetoChannel _capsulecomponent "ECC_GameTraceChannel5" "ECR_Overlap")
    (Collision|SetCollisionResponsetoChannel _capsulecomponent "ECC_GameTraceChannel2" "ECR_Overlap")
    (Collision|SetCollisionResponsetoChannel _capsulecomponent "ECC_Camera" "ECR_Ignore")))

(fn BlockCapsuleCOL
  (bind _capsulecomponent (Variables|Default|GetCapsuleComponent))
  (if (not (Utilities|Enum|Equal(Enum) (Variables|/Game/SpyroContent/Global_Assets/Global_Components/Base_AI_Character.Base_AI_Character_C|GetAICharacter_State (Variables|Default|GetWalking_AI_Character)) "NewEnumerator3"))
    (Collision|SetCollisionResponsetoChannel _capsulecomponent "ECC_Pawn" "ECR_Block")
    (Collision|SetCollisionResponsetoChannel _capsulecomponent "ECC_GameTraceChannel4" "ECR_Overlap")
    (Collision|SetCollisionResponsetoChannel _capsulecomponent "ECC_GameTraceChannel5" "ECR_Block")
    (Collision|SetCollisionResponsetoChannel _capsulecomponent "ECC_GameTraceChannel2" "ECR_Block")
    (Collision|SetCollisionResponsetoChannel _capsulecomponent "ECC_Camera" "ECR_Ignore")
    (CallFunction|GoBackUp)))

(fn DropBoxOverlapCheck
  (params (other%20actor :type Object%20Object%20Reference) (other%20comp :type Object%20Object%20Reference))
  (bind _asbp_base_playable (Utilities|Casting|CastToBP_Base_Playable other%20actor))
  (if (Math|Boolean|ANDBoolean (== (Variables|/Script/Engine.Character|GetCapsuleComponent _asbp_base_playable) other%20comp) (not (Utilities|Enum|Equal(Enum) (Variables|/Game/SpyroContent/Global_Assets/Global_Components/Base_AI_Character.Base_AI_Character_C|GetAICharacter_State (Variables|Default|GetWalking_AI_Character)) "NewEnumerator3")) (== (Variables|/Script/Engine.CharacterMovementComponent|GetGravityScale (Variables|Character|GetCharacterMovement)) 0.0) (not (Variables|Default|Getgoing%20back%20up)))
    (Variables|/Script/Engine.CharacterMovementComponent|SetGravityScale (Variables|Character|GetCharacterMovement) 4.0)
    (CallFunction|StopGoingBackUp)
    (Audio|PlaySoundatLocation "/Game/SpyroContent/CiC_Assets/CiC_Levels/Home_00_PastChasms/03_FissureFalls/LevelItems/Drop_Draklet/slide_whistle_down.slide_whistle_down" (Transformation|GetWorldLocation (Variables|Default|GetDrop_Box)) "0, 0, 0" 1.0 1.0 0.0 0 0 0)))

(fn DropBoxPing
  (bind _drop_box (Variables|Default|GetDrop_Box))
  (bind _returnvalue (Transformation|GetWorldLocation _drop_box))
  (bind _outhits (Class|KismetSystemLibrary|BoxTraceMultiforObjects _returnvalue _returnvalue "100.000000,100.000000,128.000000" "0, 0, 0" (Utilities|Array|MakeArray "ObjectTypeQuery3" "ObjectTypeQuery8" "ObjectTypeQuery9" "ObjectTypeQuery10") false 0 "None" true))
  (for _array_element _outhits
    (if (.bblockinghit _array_element)
      (CallFunction|DropBoxOverlapCheck (.hitactor _array_element) (.hitcomponent _array_element)))))