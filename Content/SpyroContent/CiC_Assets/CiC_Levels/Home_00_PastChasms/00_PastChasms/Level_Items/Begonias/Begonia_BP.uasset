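; Begonia_BP is a destructible treasure container, found in the Past Chasms home level, that acts as a begonia quest item.
; When successfully damaged, it scans every Begonia_BP actor to flag whether it is the last one destroyed.
; It then counts destroyed begonias and shows that progress against a hardcoded total in the Spyro player controller's bottom-right quest HUD.
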(event EventTreasureContainerSuccessfullyDamaged
  (|CallParentFunction)
  (Variables|Default|SetIm_The_Last_Begonia_Destroyed true)
  (bind _outactors (Actor|GetAllActorsOfClass "Begonia_BP_C"))
  (bind _array_element (Utilities|Array|ForEachLoopwithBreak _outactors :!label _label)
    (:LoopBody
      (if (and (not (== _array_element self)) (not (Variables|/Game/SpyroContent/Global_Assets/Global_Level_Items/Treasure_Containers/Treasure_Container_Base_BP.Treasure_Container_Base_BP_C|GetContainer_Destroyed _array_element)))
        (Variables|Default|SetIm_The_Last_Begonia_Destroyed false)
        (goto _label Break)))
    (:Completed
      (bind _asspyro_player_controller (Utilities|Casting|CastToSpyro_PlayerController (Game|GetPlayerController 0)))
      (bind _total_number_of_destroyed_begonias (CallFunction|CounttheBegonias))
      (Default|ShowBottomRightQuestHUD _asspyro_player_controller "/Game/SpyroContent/CiC_Assets/CiC_Levels/Home_00_PastChasms/00_PastChasms/Level_Items/Begonias/Begonia_Flipbook_Mat.Begonia_Flipbook_Mat" (Utilities|String|ToString(Integer) _total_number_of_destroyed_begonias) "7"))))

(fn ConstructionScript
  (|CallParentFunction))

(fn CounttheBegonias
  (LocalVariables|SetNumber%20of%20Destroyed%20Begonias 0)
  (bind _outactors (Actor|GetAllActorsOfClass "Begonia_BP_C"))
  (for _array_element _outactors
    (if (Variables|/Game/SpyroContent/Global_Assets/Global_Level_Items/Treasure_Containers/Treasure_Container_Base_BP.Treasure_Container_Base_BP_C|GetContainer_Destroyed _array_element)
      (Math|Integer|IncrementInt (LocalVariables|GetNumber%20of%20Destroyed%20Begonias))))
  (return (LocalVariables|GetNumber%20of%20Destroyed%20Begonias)))