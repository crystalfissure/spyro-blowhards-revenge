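; TradeItem_BP is a spittable object that serves as an item for the Arid Basin trade quest.
; On BeginPlay it binds to the Spyro_PersistantData game instance's level-unload and player-about-to-respawn events.
; Level unload destroys the actor.
; An impending respawn resets the object only if it is idle (swallowable or not), spat or broken, leaving any other state untouched.
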(event Custom|unload
  (Actor|DestroyActor))

(event Custom|reset
  (switch Utilities|FlowControl|Switch|SwitchonSpittable_Object_States (Variables|Default|GetSpittable%20Object%20State)
    (:NewEnumerator0
      _)
    (:NewEnumerator1
      _)
    (:NewEnumerator4
      _)
    (:NewEnumerator5
      _))
  (CallFunction|ResetSpittableObject))

(event EventBeginPlay
  (|CallParentFunction)
  (bind _asspyro_persistant_data (Utilities|Casting|CastToSpyro_PersistantData (Game|GetGameInstance)))
  (EventDispatchers|BindEventtoUnloadLevel _asspyro_persistant_data (delegate Custom|unload))
  (EventDispatchers|BindEventtoAnyPlayerIsAbouttoRespawn _asspyro_persistant_data (delegate Custom|reset)))

(fn ConstructionScript
  (|CallParentFunction))