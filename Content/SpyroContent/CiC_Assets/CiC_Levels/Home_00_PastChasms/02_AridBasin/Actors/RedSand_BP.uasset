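; Red sand hazard in Arid Basin that spawns an Adult Dragoid to eat and kill a player who lingers on it.
; Overlap starts a one-second retriggerable delay, then a downward trace confirms red sand, while Tick resets the timer whenever other ground is beneath.
; Invincible or supercharging players are rechecked; victims lose input, hide as the camera blends to the Dragoid, then fade out.
; Lava rocks landing on it respawn through their spawner.
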(event OnComponentBeginOverlap(hitbox)
  (params (OverlappedComponent :type Primitive%20Component%20Object%20Reference) (OtherActor :type Actor%20Object%20Reference) (OtherComp :type Primitive%20Component%20Object%20Reference) (OtherBodyIndex :type Integer) (bFromSweep :type Boolean) (SweepResult :type Hit%20Result%20Structure%20%28by%20ref%29))
  (bind _asbp_base_playable (Utilities|Casting|CastToBP_Base_Playable OtherActor)
    (:then
      (if (== (Variables|/Script/Engine.Character|GetCapsuleComponent _asbp_base_playable) OtherComp)
        (Variables|Default|Getplayer%20on%20red%20sand
          (:then)
          (:else
            (bind _output_get (Variables|Default|Setplayer%20on%20red%20sand _asbp_base_playable))
            (EventDispatchers|BindEventtoPlayerDied _output_get (delegate Custom|clear%20red%20sand%20player))
            (Utilities|FlowControl|RetriggerableDelay 1.0)
            (bind _player_on_red_sand (Variables|Default|Getplayer%20on%20red%20sand)
              (:then
                (bind _outhit (Collision|LineTraceForObjects (Transformation|GetActorLocation _player_on_red_sand) (Math|Vector|MakeVector (.X (Math|Vector|BreakVector (Transformation|GetActorLocation _player_on_red_sand))) (.Y (Math|Vector|BreakVector (Transformation|GetActorLocation _player_on_red_sand))) (- (.Z (Math|Vector|BreakVector (Transformation|GetActorLocation _player_on_red_sand))) 6e+02)) (Utilities|Array|MakeArray "ObjectTypeQuery1") false 0 "None" false))
                (if (.bblockinghit _outhit)
                  (Utilities|Casting|CastToRedSand_BP (.hitactor _outhit)
                    (:then
                      (if (and (not (Variables|/Game/SpyroContent/Global_Assets/Global_Characters/Playable_Characters/BP_Base_Playable.BP_Base_Playable_C|GetSuperinvincibility (Variables|Default|Getplayer%20on%20red%20sand))) (not (Variables|/Game/SpyroContent/Global_Assets/Global_Characters/Playable_Characters/BP_Base_Playable.BP_Base_Playable_C|GetCHEAT_Invincibility (Variables|Default|Getplayer%20on%20red%20sand))))
                        (bind _asbp_spyro (Utilities|Casting|CastToBP_Spyro (Variables|Default|Getplayer%20on%20red%20sand))
                          (:then
                            (if (Variables|/Game/SpyroContent/Global_Assets/Global_Characters/Playable_Characters/Spyro/BP_Spyro.BP_Spyro_C|Getis_Currently_Supercharging _asbp_spyro)
                              (CallFunction|TryAgain)
                              (else
                                (CallFunction|DisableThisPlayer'sInputs (Variables|Default|Getplayer%20on%20red%20sand) :!label _label)
                                (bind _returnvalue (Game|SpawnActorfromClass "/Game/SpyroContent/CiC_Assets/CiC_Levels/Home_00_PastChasms/02_AridBasin/Actors/Dragoid/Actors/AdultDragoid_BP.AdultDragoid_BP_C" (Math|Transform|MakeTransform (Math|Vector|MakeVector (.X (Math|Vector|BreakVector (.location _outhit))) (.Y (Math|Vector|BreakVector (.location _outhit))) (- (.Z (Math|Vector|BreakVector (.location _outhit))) 5e+01)) "0, 0, 0" "1,1,1") "AlwaysSpawn" 0 0))
                                (Variables|/Script/Engine.CameraComponent|SetFieldOfView (Variables|/Game/SpyroContent/CiC_Assets/CiC_Levels/Home_00_PastChasms/02_AridBasin/Actors/Dragoid/Actors/AdultDragoid_BP.AdultDragoid_BP_C|GetCamera _returnvalue) (Variables|/Script/Engine.CameraComponent|GetFieldOfView (Variables|/Game/SpyroContent/Global_Assets/Global_Characters/Playable_Characters/BP_Base_Playable.BP_Base_Playable_C|GetFollowCamera (Variables|Default|Getplayer%20on%20red%20sand))))
                                (bind _output_get_2 (Variables|Default|Setlatest%20player%20i%20ate (Variables|Default|Getplayer%20on%20red%20sand)))
                                (Game|Player|SetViewTargetwithBlend (Variables|/Game/SpyroContent/Global_Assets/Global_Characters/Playable_Characters/BP_Base_Playable.BP_Base_Playable_C|GetSpyroContr_Ref _output_get_2) _returnvalue 0.5 "VTBlend_Linear" 0.0 false)
                                (Utilities|FlowControl|Delay 0.25)
                                (bind _latest_player_i_ate (Variables|Default|Getlatest%20player%20i%20ate)
                                  (:then
                                    (Rendering|SetActorHiddenInGame _latest_player_i_ate true)
                                    (bind _current_sunglasses (Variables|/Game/SpyroContent/Global_Assets/Global_Characters/Playable_Characters/BP_Base_Playable.BP_Base_Playable_C|GetCurrent_Sunglasses _latest_player_i_ate)
                                      (:then
                                        (Rendering|SetActorHiddenInGame _current_sunglasses true))
                                      (:else
                                        _))
                                    (Utilities|FlowControl|Delay 1.0)
                                    (bind _latest_player_i_ate_2 (Variables|Default|Getlatest%20player%20i%20ate)
                                      (:then
                                        (Default|InvokedResetCamera _latest_player_i_ate_2)
                                        (CameraFades|StartCameraFade :self (Variables|/Script/Engine.PlayerController|GetPlayerCameraManager (Variables|/Game/SpyroContent/Global_Assets/Global_Characters/Playable_Characters/BP_Base_Playable.BP_Base_Playable_C|GetSpyroContr_Ref _latest_player_i_ate_2)) :ToAlpha 1.0 :Duration 0.5 :bShouldFadeAudio true :bHoldWhenFinished true)
                                        (Variables|/Game/SpyroContent/Global_Assets/Global_Characters/Playable_Characters/BP_Base_Playable.BP_Base_Playable_C|Setkill%20player%20-%20dont%20set%20view%20target (Variables|Default|Getlatest%20player%20i%20ate) true)
                                        (Variables|/Game/SpyroContent/Global_Assets/Global_Characters/Playable_Characters/BP_Base_Playable.BP_Base_Playable_C|SetDeath_Delay (Variables|Default|Getlatest%20player%20i%20ate) 0.0)
                                        (if (Variables|/Game/SpyroContent/Global_Assets/Global_Characters/Playable_Characters/BP_Base_Playable.BP_Base_Playable_C|GetFairyFall (Variables|Default|Getlatest%20player%20i%20ate))
                                          (Variables|/Game/SpyroContent/Global_Assets/Global_Characters/Playable_Characters/BP_Base_Playable.BP_Base_Playable_C|Setcurrently%20fairy%20falling (Variables|Default|Getlatest%20player%20i%20ate) true))
                                        (Default|KillPlayer (Variables|Default|Getlatest%20player%20i%20ate) "NewEnumerator4")
                                        (Utilities|FlowControl|Delay 0.5)
                                        (Rendering|SetActorHiddenInGame (Variables|Default|Getlatest%20player%20i%20ate) false)
                                        (Variables|Default|Setlatest%20player%20i%20ate 0))
                                      (:else)))
                                  (:else)))))
                          (:CastFailed
                            (goto _label)))
                        (else
                          (CallFunction|TryAgain))))
                    (:CastFailed
                      (Variables|Default|Setplayer%20on%20red%20sand 0)))
                  (else
                    (CallFunction|TryAgain))))
              (:else))))))
    (:CastFailed
      (bind _aslava_rock_bp (Utilities|Casting|CastToLavaRock_BP OtherActor))
      (switch Utilities|FlowControl|Switch|SwitchonSpittable_Object_States (Variables|/Game/SpyroContent/Global_Assets/Global_Level_Items/Spittable_Object/Base_Spittable_Object_BP.Base_Spittable_Object_BP_C|GetSpittable%20Object%20State _aslava_rock_bp)
        (:NewEnumerator0
          _)
        (:NewEnumerator1
          _))
      (Default|SpawnLavaRock (Variables|/Game/SpyroContent/Global_Assets/Global_Level_Items/Spittable_Object/LavaRock/LavaRock_BP.LavaRock_BP_C|GetMy%20Spawner _aslava_rock_bp))
      (Actor|DestroyActor _aslava_rock_bp))))

(event Custom|clear%20red%20sand%20player
  (Variables|Default|Setplayer%20on%20red%20sand 0))

(event Custom|try%20again
  (Utilities|FlowControl|RetriggerableDelay 1.0)
  (bind _player_on_red_sand (Variables|Default|Getplayer%20on%20red%20sand)
    (:then
      (bind _outhit (Collision|LineTraceForObjects (Transformation|GetActorLocation _player_on_red_sand) (Math|Vector|MakeVector (.X (Math|Vector|BreakVector (Transformation|GetActorLocation _player_on_red_sand))) (.Y (Math|Vector|BreakVector (Transformation|GetActorLocation _player_on_red_sand))) (- (.Z (Math|Vector|BreakVector (Transformation|GetActorLocation _player_on_red_sand))) 6e+02)) (Utilities|Array|MakeArray "ObjectTypeQuery1") false 0 "None" false))
      (if (.bblockinghit _outhit)
        (Utilities|Casting|CastToRedSand_BP (.hitactor _outhit)
          (:then
            (if (and (not (Variables|/Game/SpyroContent/Global_Assets/Global_Characters/Playable_Characters/BP_Base_Playable.BP_Base_Playable_C|GetSuperinvincibility (Variables|Default|Getplayer%20on%20red%20sand))) (not (Variables|/Game/SpyroContent/Global_Assets/Global_Characters/Playable_Characters/BP_Base_Playable.BP_Base_Playable_C|GetCHEAT_Invincibility (Variables|Default|Getplayer%20on%20red%20sand))))
              (bind _asbp_spyro (Utilities|Casting|CastToBP_Spyro (Variables|Default|Getplayer%20on%20red%20sand))
                (:then
                  (if (Variables|/Game/SpyroContent/Global_Assets/Global_Characters/Playable_Characters/Spyro/BP_Spyro.BP_Spyro_C|Getis_Currently_Supercharging _asbp_spyro)
                    (CallFunction|TryAgain)
                    (else
                      (CallFunction|DisableThisPlayer'sInputs (Variables|Default|Getplayer%20on%20red%20sand) :!label _label)
                      (bind _returnvalue (Game|SpawnActorfromClass "/Game/SpyroContent/CiC_Assets/CiC_Levels/Home_00_PastChasms/02_AridBasin/Actors/Dragoid/Actors/AdultDragoid_BP.AdultDragoid_BP_C" (Math|Transform|MakeTransform (Math|Vector|MakeVector (.X (Math|Vector|BreakVector (.location _outhit))) (.Y (Math|Vector|BreakVector (.location _outhit))) (- (.Z (Math|Vector|BreakVector (.location _outhit))) 5e+01)) "0, 0, 0" "1,1,1") "AlwaysSpawn" 0 0))
                      (Variables|/Script/Engine.CameraComponent|SetFieldOfView (Variables|/Game/SpyroContent/CiC_Assets/CiC_Levels/Home_00_PastChasms/02_AridBasin/Actors/Dragoid/Actors/AdultDragoid_BP.AdultDragoid_BP_C|GetCamera _returnvalue) (Variables|/Script/Engine.CameraComponent|GetFieldOfView (Variables|/Game/SpyroContent/Global_Assets/Global_Characters/Playable_Characters/BP_Base_Playable.BP_Base_Playable_C|GetFollowCamera (Variables|Default|Getplayer%20on%20red%20sand))))
                      (bind _output_get (Variables|Default|Setlatest%20player%20i%20ate (Variables|Default|Getplayer%20on%20red%20sand)))
                      (Game|Player|SetViewTargetwithBlend (Variables|/Game/SpyroContent/Global_Assets/Global_Characters/Playable_Characters/BP_Base_Playable.BP_Base_Playable_C|GetSpyroContr_Ref _output_get) _returnvalue 0.5 "VTBlend_Linear" 0.0 false)
                      (Utilities|FlowControl|Delay 0.25)
                      (bind _latest_player_i_ate (Variables|Default|Getlatest%20player%20i%20ate)
                        (:then
                          (Rendering|SetActorHiddenInGame _latest_player_i_ate true)
                          (bind _current_sunglasses (Variables|/Game/SpyroContent/Global_Assets/Global_Characters/Playable_Characters/BP_Base_Playable.BP_Base_Playable_C|GetCurrent_Sunglasses _latest_player_i_ate)
                            (:then
                              (Rendering|SetActorHiddenInGame _current_sunglasses true))
                            (:else
                              _))
                          (Utilities|FlowControl|Delay 1.0)
                          (bind _latest_player_i_ate_2 (Variables|Default|Getlatest%20player%20i%20ate)
                            (:then
                              (Default|InvokedResetCamera _latest_player_i_ate_2)
                              (CameraFades|StartCameraFade :self (Variables|/Script/Engine.PlayerController|GetPlayerCameraManager (Variables|/Game/SpyroContent/Global_Assets/Global_Characters/Playable_Characters/BP_Base_Playable.BP_Base_Playable_C|GetSpyroContr_Ref _latest_player_i_ate_2)) :ToAlpha 1.0 :Duration 0.5 :bShouldFadeAudio true :bHoldWhenFinished true)
                              (Variables|/Game/SpyroContent/Global_Assets/Global_Characters/Playable_Characters/BP_Base_Playable.BP_Base_Playable_C|Setkill%20player%20-%20dont%20set%20view%20target (Variables|Default|Getlatest%20player%20i%20ate) true)
                              (Variables|/Game/SpyroContent/Global_Assets/Global_Characters/Playable_Characters/BP_Base_Playable.BP_Base_Playable_C|SetDeath_Delay (Variables|Default|Getlatest%20player%20i%20ate) 0.0)
                              (if (Variables|/Game/SpyroContent/Global_Assets/Global_Characters/Playable_Characters/BP_Base_Playable.BP_Base_Playable_C|GetFairyFall (Variables|Default|Getlatest%20player%20i%20ate))
                                (Variables|/Game/SpyroContent/Global_Assets/Global_Characters/Playable_Characters/BP_Base_Playable.BP_Base_Playable_C|Setcurrently%20fairy%20falling (Variables|Default|Getlatest%20player%20i%20ate) true))
                              (Default|KillPlayer (Variables|Default|Getlatest%20player%20i%20ate) "NewEnumerator4")
                              (Utilities|FlowControl|Delay 0.5)
                              (Rendering|SetActorHiddenInGame (Variables|Default|Getlatest%20player%20i%20ate) false)
                              (Variables|Default|Setlatest%20player%20i%20ate 0))
                            (:else)))
                        (:else)))))
                (:CastFailed
                  (goto _label)))
              (else
                (CallFunction|TryAgain))))
          (:CastFailed
            (Variables|Default|Setplayer%20on%20red%20sand 0)))
        (else
          (CallFunction|TryAgain))))
    (:else)))

(event EventTick
  (params (DeltaSeconds :type Float%20%28single-precision%29))
  (bind _player_on_red_sand (Variables|Default|Getplayer%20on%20red%20sand)
    (:then
      (bind _outhit (Collision|LineTraceForObjects (Transformation|GetActorLocation _player_on_red_sand) (Math|Vector|MakeVector (.X (Math|Vector|BreakVector (Transformation|GetActorLocation _player_on_red_sand))) (.Y (Math|Vector|BreakVector (Transformation|GetActorLocation _player_on_red_sand))) (- (.Z (Math|Vector|BreakVector (Transformation|GetActorLocation _player_on_red_sand))) 6e+02)) (Utilities|Array|MakeArray "ObjectTypeQuery1") false 0 "None" false))
      (if (.bblockinghit _outhit)
        (Utilities|Casting|CastToRedSand_BP (.hitactor _outhit)
          (:CastFailed
            (if (AI|Components|NavMovement|IsFalling (Variables|/Script/Engine.Character|GetCharacterMovement (Variables|Default|Getplayer%20on%20red%20sand)))
              (Variables|Default|Setplayer%20on%20red%20sand 0))
            (CallFunction|TryAgain)))))
    (:else)))

(fn ConstructionScript)