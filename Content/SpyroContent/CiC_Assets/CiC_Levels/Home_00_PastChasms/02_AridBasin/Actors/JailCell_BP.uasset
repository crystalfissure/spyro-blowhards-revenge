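; Breakable metal jail cell actor that glows when heated and bursts into shards when damaged.
; Its Damageable component triggers a heat timeline that animates the dynamic material's ColorChange parameter, with a DoOnce gate that resets after a short delay.
; When damage meets DamageRequirement, it spawns reused basket burst actors once, offset above, below, left and right, each throwing the cell's shard meshes.
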(event EventBeginPlay
  (bind _damageable (Variables|Default|GetDamageable))
  (bind _staticmesh1 (Variables|Default|GetStaticMesh1))
  (|CallParentFunction)
  (Variables|/Game/SpyroContent/Global_Assets/Global_Components/Damageable_Com.Damageable_Com_C|SetComponent_with_Metal_Material _damageable (Variables|Default|GetStaticMesh1))
  (EventDispatchers|BindEventtoHeatMetal _damageable (|HeattheMetal))
  (bind _returnvalue (Rendering|Material|CreateDynamicMaterialInstance _staticmesh1 0 (Rendering|Material|GetMaterial _staticmesh1 0) "None" :!class /Script/Engine.PrimitiveComponent))
  (Variables|Default|Setdyn%20mat%20ref _returnvalue))

(event EventOnDamaged
  (bind _returnvalue (Transformation|GetActorTransform))
  (bind _returnvalue_2 (Transformation|GetActorTransform))
  (bind _returnvalue_3 (Transformation|GetActorTransform))
  (bind _returnvalue_4 (Transformation|GetActorTransform))
  (|CallParentFunction)
  (bind _returnvalue_5 (CallFunction|DamageRequirement))
  (if _returnvalue_5
    (Utilities|FlowControl|DoOnce false
      (:Completed
        (bind _returnvalue_6 (Game|SpawnActorfromClass "/Game/SpyroContent/Global_Assets/Global_Level_Items/Treasure_Containers/Basket/Actors/Basket_Burst_BP.Basket_Burst_BP_C" (Math|Transform|MakeTransform (+ (.location _returnvalue_4) (* (Transformation|GetActorUpVector) 3e+02)) (.rotation _returnvalue_4) (.scale _returnvalue_4)) "AdjustIfPossibleButAlwaysSpawn" 0 0))
        (Default|ShardBurstAction _returnvalue_6 (Variables|Default|GetShard%20Mesh%201) (Variables|Default|GetShard%20Mesh%202))
        (bind _returnvalue_7 (Game|SpawnActorfromClass "/Game/SpyroContent/Global_Assets/Global_Level_Items/Treasure_Containers/Basket/Actors/Basket_Burst_BP.Basket_Burst_BP_C" (Math|Transform|MakeTransform (+ (.location _returnvalue_2) (* (Transformation|GetActorUpVector) -3e+02)) (.rotation _returnvalue_2) (.scale _returnvalue_2)) "AdjustIfPossibleButAlwaysSpawn" 0 0))
        (Default|ShardBurstAction _returnvalue_7 (Variables|Default|GetShard%20Mesh%201) (Variables|Default|GetShard%20Mesh%202))
        (bind _returnvalue_8 (Game|SpawnActorfromClass "/Game/SpyroContent/Global_Assets/Global_Level_Items/Treasure_Containers/Basket/Actors/Basket_Burst_BP.Basket_Burst_BP_C" (Math|Transform|MakeTransform (+ (.location _returnvalue_3) (* (Transformation|GetActorRightVector) -3e+02)) (.rotation _returnvalue_3) (.scale _returnvalue_3)) "AdjustIfPossibleButAlwaysSpawn" 0 0))
        (Default|ShardBurstAction _returnvalue_8 (Variables|Default|GetShard%20Mesh%201) (Variables|Default|GetShard%20Mesh%202))
        (bind _returnvalue_9 (Game|SpawnActorfromClass "/Game/SpyroContent/Global_Assets/Global_Level_Items/Treasure_Containers/Basket/Actors/Basket_Burst_BP.Basket_Burst_BP_C" (Math|Transform|MakeTransform (+ (.location _returnvalue) (* (Transformation|GetActorRightVector) 3e+02)) (.rotation _returnvalue) (.scale _returnvalue)) "AdjustIfPossibleButAlwaysSpawn" 0 0))
        (Default|ShardBurstAction _returnvalue_9 (Variables|Default|GetShard%20Mesh%201) (Variables|Default|GetShard%20Mesh%202))))))

(fn ConstructionScript
  (|CallParentFunction))

(event Custom|Reset%20Heat%20Metal
  (Utilities|FlowControl|DoOnce false) ; enters at Reset
)

(event Custom|Heat%20Metal
  (Utilities|FlowControl|DoOnce false
    (:Completed
      (Utilities|FlowControl|Sequence
        (:then_0
          (bind _newtrack_0 (Timeline|Timeline_0 PlayFromStart)
            (:Update
              (bind _dyn_mat_ref (Variables|Default|Getdyn%20mat%20ref)
                (:then
                  (Rendering|Material|SetVectorParameterValue _dyn_mat_ref "ColorChange" (Utilities|Struct|MakeLinearColor (.x _newtrack_0) (.y _newtrack_0) (.z _newtrack_0) 0.0) :!class /Script/Engine.MaterialInstanceDynamic))
                (:else)))))
        (:then_1
          (Utilities|FlowControl|Delay 1.0)
          (CallFunction|ResetHeatMetal))))))