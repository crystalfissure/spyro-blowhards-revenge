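; Monkey NPC for N. Sanity Beach that hops repeatedly while the player is nearby.
; HopRadius overlaps start and stop a looping jump timer, backed by a periodic box trace; frozen or fear-paralyzed monkeys skip jumps.
; When falling onto the player it launches them away, and spittable objects hit below it are teleported in front.
; The drop shadow uses absolute transforms to stay put during hops.
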(event OnComponentBeginOverlap(hopradius)
  (params (OverlappedComponent :type Primitive%20Component%20Object%20Reference) (OtherActor :type Actor%20Object%20Reference) (OtherComp :type Primitive%20Component%20Object%20Reference) (OtherBodyIndex :type Integer) (bFromSweep :type Boolean) (SweepResult :type Hit%20Result%20Structure%20%28by%20ref%29))
  (bind _asbp_base_playable (Utilities|Casting|CastToBP_Base_Playable OtherActor))
  (if (and (== (Variables|/Script/Engine.Character|GetCapsuleComponent _asbp_base_playable) OtherComp) (not (Utilities|Time|IsValidTimerHandle (Variables|Default|Gethop%20timer))))
    (bind _returnvalue (Utilities|Time|SetTimerbyFunctionName 0 "hop" 0.5 true))
    (Variables|Default|Sethop%20timer _returnvalue)))

(event OnComponentEndOverlap(hopradius)
  (params (OverlappedComponent :type Primitive%20Component%20Object%20Reference) (OtherActor :type Actor%20Object%20Reference) (OtherComp :type Primitive%20Component%20Object%20Reference) (OtherBodyIndex :type Integer))
  (bind _asbp_base_playable (Utilities|Casting|CastToBP_Base_Playable OtherActor))
  (if (and (== (Variables|/Script/Engine.Character|GetCapsuleComponent _asbp_base_playable) OtherComp) (Utilities|Time|IsValidTimerHandle (Variables|Default|Gethop%20timer)))
    (Utilities|Time|ClearandInvalidateTimerbyHandle (Variables|Default|Gethop%20timer))))

(event OnComponentHit(CapsuleComponent)
  (params (HitComponent :type Primitive%20Component%20Object%20Reference) (OtherActor :type Actor%20Object%20Reference) (OtherComp :type Primitive%20Component%20Object%20Reference) (NormalImpulse :type Vector :default "0, 0, 0") (Hit :type Hit%20Result%20Structure%20%28by%20ref%29))
  (bind _returnvalue (Transformation|GetActorForwardVector))
  (bind _returnvalue_2 (Transformation|GetActorLocation))
  (bind _returnvalue_3 (* _returnvalue 1e+02))
  (bind _returnvalue_4 (+ _returnvalue_2 _returnvalue_3))
  (bind _asbp_base_playable (Utilities|Casting|CastToBP_Base_Playable OtherActor)
    (:then
      (if (Math|Boolean|ANDBoolean (== (Variables|/Script/Engine.Character|GetCapsuleComponent _asbp_base_playable) OtherComp) (AI|Components|NavMovement|IsFalling (Variables|Character|GetCharacterMovement)) (< (.z (Transformation|GetActorLocation _asbp_base_playable)) (.z (Transformation|GetActorLocation))))
        (Character|LaunchCharacter _asbp_base_playable (Math|Vector|MakeVector (.x (* (Math|Vector|GetForwardVector (Math|Rotator|MakeRotator 0.0 0.0 (.yaw (Math|Rotator|FindLookatRotation (Transformation|GetActorLocation) (Transformation|GetActorLocation _asbp_base_playable))))) 3e+02)) (.y (* (Math|Vector|GetForwardVector (Math|Rotator|MakeRotator 0.0 0.0 (.yaw (Math|Rotator|FindLookatRotation (Transformation|GetActorLocation) (Transformation|GetActorLocation _asbp_base_playable))))) 3e+02)) (+ (.z (* (Math|Vector|GetForwardVector (Math|Rotator|MakeRotator 0.0 0.0 (.yaw (Math|Rotator|FindLookatRotation (Transformation|GetActorLocation) (Transformation|GetActorLocation _asbp_base_playable))))) 3e+02)) 3e+02)) true true)))
    (:CastFailed
      (bind _asbase_spittable_object_bp (Utilities|Casting|CastToBase_Spittable_Object_BP OtherActor))
      (if (< (.z (Transformation|GetActorLocation _asbase_spittable_object_bp)) (.z (Transformation|GetActorLocation)))
        (Transformation|SetActorLocation _asbase_spittable_object_bp (Math|Vector|MakeVector (.x _returnvalue_4) (.y _returnvalue_4) (+ (.z (Transformation|GetWorldLocation (Variables|Default|GetDropshadow))) 2e+01)) false true)))))

(event EventBeginPlay
  (bind _dropshadow (Variables|Default|GetDropshadow))
  (|CallParentFunction)
  (Utilities|Time|SetTimerbyFunctionName 0 "hop ping" 0.5 true)
  (Variables|Default|Setdropshadow%20transf (Transformation|GetWorldTransform _dropshadow))
  (Transformation|SetAbsolute _dropshadow true true true)
  (Transformation|SetWorldTransform (Variables|Default|GetDropshadow) (Variables|Default|Getdropshadow%20transf) false false)
  (Variables|/Game/SpyroContent/Global_Assets/Global_Components/Damageable_Com.Damageable_Com_C|SetObject's%20Hitbox%20Component (Variables|Default|GetNPC_Damageable) (Variables|Default|Gethitbox)))

(fn ConstructionScript
  (|CallParentFunction))

(fn Hop
  (bind _npc_damageable (Variables|Default|GetNPC_Damageable))
  (if (Math|Boolean|ANDBoolean (not (AI|Components|NavMovement|IsFalling (Variables|Character|GetCharacterMovement))) (not (Variables|/Game/SpyroContent/Global_Assets/Global_Components/Damageable_Com.Damageable_Com_C|GetFrozen _npc_damageable)) (not (Variables|/Game/SpyroContent/Global_Assets/Global_Components/Damageable_Com.Damageable_Com_C|GetParalyzed_by_Fear _npc_damageable)))
    (Character|Jump)
    (Development|PrintString "hop!")))

(fn HopPing
  (bind _hop_radius (Variables|Default|Gethop%20radius))
  (bind _returnvalue (Transformation|GetWorldLocation _hop_radius))
  (bind _boxextent (Variables|/Script/Engine.BoxComponent|GetBoxExtent _hop_radius))
  (bind _outhits (Class|KismetSystemLibrary|BoxTraceMultiforObjects _returnvalue _returnvalue (Math|Vector|MakeVector (.x _boxextent) (.x _boxextent) (.x _boxextent)) (Transformation|GetWorldRotation _hop_radius) (Utilities|Array|MakeArray "ObjectTypeQuery3" "ObjectTypeQuery9" "ObjectTypeQuery8" "ObjectTypeQuery10") false 0 "None" true))
  (for _array_element _outhits
    (bind _asbp_base_playable (Utilities|Casting|CastToBP_Base_Playable (.hitactor _array_element)))
    (if (and (== (Variables|/Script/Engine.Character|GetCapsuleComponent _asbp_base_playable) (.hitcomponent _array_element)) (not (Utilities|Time|IsValidTimerHandle (Variables|Default|Gethop%20timer))))
      (bind _returnvalue_2 (Utilities|Time|SetTimerbyFunctionName 0 "hop" 0.5 true))
      (Variables|Default|Sethop%20timer _returnvalue_2))))