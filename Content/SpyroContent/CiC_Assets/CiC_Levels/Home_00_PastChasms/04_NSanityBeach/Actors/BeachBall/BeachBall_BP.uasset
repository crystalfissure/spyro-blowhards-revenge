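; Physics beach ball for the N. Sanity Beach level that players can knock around and that damages other objects it touches.
; Player contact and incoming damage add impulses to the sphere, with stronger launches for Ram.
; A looping box trace deals Ram damage to nearby non-player damageables, while physics hits deal Crush.
; It resets on water hits or player respawn, and a downward trace keeps a plane on the ground beneath it.
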(event OnComponentHit(Sphere)
  (params (HitComponent :type Primitive%20Component%20Object%20Reference) (OtherActor :type Actor%20Object%20Reference) (OtherComp :type Primitive%20Component%20Object%20Reference) (NormalImpulse :type Vector :default "0, 0, 0") (Hit :type Hit%20Result%20Structure%20%28by%20ref%29))
  (bind _returnvalue (Actor|GetComponentbyClass OtherActor "/Game/SpyroContent/Global_Assets/Global_Components/Damageable_Com.Damageable_Com_C"))
  (bind _asbp_base_playable (Utilities|Casting|CastToBP_Base_Playable OtherActor)
    (:then
      (if (== (Variables|/Script/Engine.Character|GetCapsuleComponent _asbp_base_playable) OtherComp)
        (Physics|AddImpulse (Variables|Default|GetSphere) (Math|Vector|MakeVector (.x (* (Transformation|GetActorForwardVector OtherActor) (select (Utilities|Enum|Equal(Enum) (Variables|/Game/SpyroContent/Global_Assets/Global_Characters/Playable_Characters/BP_Base_Playable.BP_Base_Playable_C|GetPlayer_State _asbp_base_playable) "NewEnumerator4") 99999.0 9999.0))) (.y (* (Transformation|GetActorForwardVector OtherActor) (select (Utilities|Enum|Equal(Enum) (Variables|/Game/SpyroContent/Global_Assets/Global_Characters/Playable_Characters/BP_Base_Playable.BP_Base_Playable_C|GetPlayer_State _asbp_base_playable) "NewEnumerator4") 99999.0 9999.0))) (+ (.z (* (Transformation|GetActorForwardVector OtherActor) (select (Utilities|Enum|Equal(Enum) (Variables|/Game/SpyroContent/Global_Assets/Global_Characters/Playable_Characters/BP_Base_Playable.BP_Base_Playable_C|GetPlayer_State _asbp_base_playable) "NewEnumerator4") 99999.0 9999.0))) (select (Utilities|Enum|Equal(Enum) (Variables|/Game/SpyroContent/Global_Assets/Global_Characters/Playable_Characters/BP_Base_Playable.BP_Base_Playable_C|GetPlayer_State _asbp_base_playable) "NewEnumerator4") 9999.0 0.0))) "None" false)))
    (:CastFailed
      (Utilities|Casting|CastToDrownable_Water_BP OtherActor
        (:then
          (CallFunction|ResetSphere))
        (:CastFailed
          (Utilities|IsValid _returnvalue
            (:Is%20Valid
              (Default|DealDamage _returnvalue "NewEnumerator2" "0, 0, 0" true 0 false))))))))

(event Custom|On%20Damaged
  (bind _returnvalue (Transformation|GetActorForwardVector))
  (bind _damageable_com (Variables|Default|GetDamageable_Com))
  (bind _returnvalue_2 (* _returnvalue 3e+05))
  (Default|CallDamageWasSuccessfullyDealt (Variables|Default|GetDamageable_Com))
  (bind _deal_damage___person_who_dealt_the_damage (Variables|/Game/SpyroContent/Global_Assets/Global_Components/Damageable_Com.Damageable_Com_C|GetDeal%20Damage%20-%20Person%20Who%20Dealt%20the%20Damage _damageable_com)
    (:then
      (switch Utilities|FlowControl|Switch|SwitchonDamage_Types (Variables|/Game/SpyroContent/Global_Assets/Global_Components/Damageable_Com.Damageable_Com_C|GetDeal%20Damage%20-%20Damage%20Type _damageable_com)
        (:NewEnumerator0
          _)
        (:NewEnumerator1
          _)
        (:NewEnumerator2
          _)
        (:NewEnumerator3
          _)
        (:NewEnumerator4
          (Utilities|FlowControl|DoOnce false :!label _label
            (:Completed
              (Physics|AddImpulse (Variables|Default|GetSphere) (Math|Vector|MakeVector (.x _returnvalue_2) (.y _returnvalue_2) (+ (.z _returnvalue_2) 9999.0)) "None" false)
              (Utilities|FlowControl|Delay 0.5)
              (goto _label Reset))))
        (:NewEnumerator5
          _)
        (:NewEnumerator7
          _)
        (:NewEnumerator8
          _)
        (:NewEnumerator9
          _)
        (:NewEnumerator10
          _)
        (:NewEnumerator11
          _)
        (:NewEnumerator12
          _)
        (:NewEnumerator13
          _))
      (Utilities|FlowControl|DoOnce false :!label _label_2
        (:Completed
          (Physics|AddImpulse (Variables|Default|GetSphere) (* (Transformation|GetActorForwardVector _deal_damage___person_who_dealt_the_damage) 2e+05) "None" false)
          (Utilities|FlowControl|Delay 0.5)
          (goto _label_2 Reset))))
    (:else)))

(event Custom|reset%20sphere
  (bind _returnvalue (Transformation|GetActorLocation))
  (bind _returnvalue_2 (Transformation|GetActorLocation))
  (Effects|SpawnEmitteratLocation "/Game/SpyroContent/Global_Assets/Global_Particles/dust_ring.dust_ring" _returnvalue_2 "0, 0, 0" "0.500000,0.500000,0.500000")
  (Audio|PlaySoundatLocation "/Game/SpyroContent/Global_Assets/Global_Characters/AI_Characters/death_poof_s1.death_poof_s1" _returnvalue_2 "0, 0, 0" 1.0 1.0 0.0 0 0 0)
  (Transformation|SetActorLocation (Variables|Default|Getstarting%20location) false false)
  (Physics|SetSimulatePhysics (Variables|Default|GetSphere) false)
  (Effects|SpawnEmitteratLocation "/Game/SpyroContent/Global_Assets/Global_Particles/dust_ring.dust_ring" _returnvalue "0, 0, 0" "0.500000,0.500000,0.500000")
  (Audio|PlaySoundatLocation "/Game/SpyroContent/Global_Assets/Global_Characters/AI_Characters/death_poof_s1.death_poof_s1" _returnvalue "0, 0, 0" 1.0 1.0 0.0 0 0 0)
  (Utilities|FlowControl|Delay 0.2)
  (Physics|SetSimulatePhysics (Variables|Default|GetSphere) true))

(event EventBeginPlay
  (bind _damageable_com (Variables|Default|GetDamageable_Com))
  (Utilities|Time|SetTimerbyFunctionName 0 "damage ping" 0.2 true)
  (Variables|Default|Setstarting%20location (Transformation|GetActorLocation))
  (bind _asspyro_persistant_data (Utilities|Casting|CastToSpyro_PersistantData (Game|GetGameInstance)))
  (EventDispatchers|BindEventtoAnyPlayerIsAbouttoRespawn _asspyro_persistant_data (delegate Custom|reset%20sphere))
  (Variables|/Game/SpyroContent/Global_Assets/Global_Components/Damageable_Com.Damageable_Com_C|SetObject's%20Hitbox%20Component _damageable_com (Variables|Default|GetBox))
  (EventDispatchers|BindEventtoCallDealDamage _damageable_com (delegate Custom|On%20Damaged)))

(event EventTick
  (params (DeltaSeconds :type Float%20%28single-precision%29))
  (bind _returnvalue (Transformation|GetActorLocation))
  (bind (_x _y _z) (Math|Vector|BreakVector _returnvalue))
  (bind _outhit (Collision|LineTraceForObjects _returnvalue (Math|Vector|MakeVector _x _y (- _z 99999.0)) (Utilities|Array|MakeArray "ObjectTypeQuery1") false 0 "None"))
  (if (.bblockinghit _outhit)
    (Transformation|SetWorldLocation (Variables|Default|GetPlane) (Math|Vector|MakeVector (.x (.location _outhit)) (.y (.location _outhit)) (+ (.z (.location _outhit)) 5.0)) false false)))

(fn ConstructionScript)

(fn DamagePing
  (bind _returnvalue (Transformation|GetActorLocation))
  (bind _outhits (Class|KismetSystemLibrary|BoxTraceMultiforObjects _returnvalue _returnvalue "60.000000,60.000000,60.000000" "0, 0, 0" (Utilities|Array|MakeArray "ObjectTypeQuery1" "ObjectTypeQuery2" "ObjectTypeQuery3") false 0 "None" true))
  (for _array_element _outhits
    (Utilities|Casting|CastToBP_Base_Playable (.hitactor _array_element)
      (:CastFailed
        (Utilities|IsValid (Actor|GetComponentbyClass (.hitactor _array_element) "/Game/SpyroContent/Global_Assets/Global_Components/Damageable_Com.Damageable_Com_C")
          (:Is%20Valid
            (Default|DealDamage (Actor|GetComponentbyClass (.hitactor _array_element) "/Game/SpyroContent/Global_Assets/Global_Components/Damageable_Com.Damageable_Com_C") "NewEnumerator4" "0, 0, 0" true 0 false)))))))