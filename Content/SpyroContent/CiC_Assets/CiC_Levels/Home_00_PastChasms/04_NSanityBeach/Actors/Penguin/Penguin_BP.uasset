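; Penguin enemy for the N. Sanity Beach level, with a spin attack that shuttles it between its spawn point and a SpinToHere marker.
; While the spin mesh is visible, Tick lerps it horizontally at a difficulty-based speed, and a looping timer sphere-traces to damage nearby Damageable actors.
; Idle, Alert or Dying states restore the normal mesh and stop spin damage and audio.
; Freezing, or fear from a specific damage type, drops an attacking penguin to Idle.
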(event Custom|penguin%20state%20changed
  (switch Utilities|FlowControl|Switch|SwitchonAICharacter_States (Variables|/Game/SpyroContent/Global_Assets/Global_Components/Base_AI_Character.Base_AI_Character_C|GetAICharacter_State (Variables|Default|GetWalking_AI_Character))
    (:NewEnumerator0
      _)
    (:NewEnumerator1
      _)
    (:NewEnumerator3
      _))
  (Rendering|SetVisibility (Variables|Default|Getspin_mesh) false false)
  (Rendering|SetVisibility (Variables|Character|GetMesh) true false)
  (Utilities|Time|ClearandInvalidateTimerbyHandle (Variables|Default|Getspin%20damage%20timer))
  (Utilities|Array|RemoveItem (Variables|/Game/SpyroContent/Global_Assets/Global_Components/Damageable_Com.Damageable_Com_C|GetDamage_Resistances (Variables|Default|GetDamageable)) "NewEnumerator4")
  (Collision|SetCollisionResponsetoChannel (Variables|Default|GetCapsuleComponent) "ECC_GameTraceChannel4" "ECR_Overlap")
  (Audio|Components|Audio|Stop (Variables|Default|Getspin_Audio)))

(event Custom|spin%20damage%20time%20start
  (bind _returnvalue (Utilities|Time|SetTimerbyFunctionName 0 "spin damage" 0.2 true))
  (Variables|Default|Setspin%20damage%20timer _returnvalue)
  (Audio|Components|Audio|Play (Variables|Default|Getspin_Audio) 0.0))

(event Custom|freeze%20penguin
  (bind _walking_ai_character (Variables|Default|GetWalking_AI_Character))
  (switch Utilities|FlowControl|Switch|SwitchonAICharacter_States (Variables|/Game/SpyroContent/Global_Assets/Global_Components/Base_AI_Character.Base_AI_Character_C|GetAICharacter_State _walking_ai_character)
    (:NewEnumerator2
      (Default|ChangeAICharacterState _walking_ai_character "NewEnumerator0"))))

(event Custom|on%20penguin%20reset
  (Variables|Default|Setspinning%20home false))

(event EventBeginPlay
  (|CallParentFunction)
  (EventDispatchers|BindEventtoMyStateChanged (Variables|Default|GetWalking_AI_Character) (delegate Custom|penguin%20state%20changed))
  (EventDispatchers|BindEventtoCallFreeze (Variables|Default|GetDamageable) (delegate Custom|freeze%20penguin))
  (Variables|Default|Setspin%20destination (Transformation|GetWorldLocation (Variables|Default|Getspin%20to%20here)))
  (EventDispatchers|BindEventtoItemDropperSuccessfullyReset (Variables|Default|GetDrops_Items) (delegate Custom|on%20penguin%20reset)))

(event EventTick
  (params (DeltaSeconds :type Float%20%28single-precision%29))
  (bind _returnvalue (Transformation|GetActorLocation))
  (bind _returnvalue_2 (Transformation|GetActorLocation))
  (bind _returnvalue_3 (Transformation|GetActorLocation))
  (bind _medium_walk_speed (Variables|Default|GetMedium%20Walk%20Speed))
  (bind _spin_destination (Variables|Default|Getspin%20destination))
  (bind _walking_ai_character (Variables|Default|GetWalking_AI_Character))
  (bind _spin_destination_2 (Variables|Default|Getspin%20destination))
  (bind _walking_ai_character_2 (Variables|Default|GetWalking_AI_Character))
  (bind _damageable (Variables|Default|GetDamageable))
  (bind _walking_ai_character_3 (Variables|Default|GetWalking_AI_Character))
  (bind _spawn_point (Variables|/Game/SpyroContent/Global_Assets/Global_Components/Base_AI_Character.Base_AI_Character_C|GetSpawn_Point _walking_ai_character))
  (bind _spawn_point_2 (Variables|/Game/SpyroContent/Global_Assets/Global_Components/Base_AI_Character.Base_AI_Character_C|GetSpawn_Point _walking_ai_character_2))
  (if (Utilities|Enum|Equal(Enum) (Variables|/Game/SpyroContent/Global_Assets/Global_Components/Base_AI_Character.Base_AI_Character_C|GetAICharacter_State (Variables|Default|GetWalking_AI_Character)) "NewEnumerator3")
    (if (Variables|Default|Getspinning%20home)
      (Variables|Default|Setspinning%20home false))
    (elif (and (not (Variables|/Game/SpyroContent/Global_Assets/Global_Components/Damageable_Com.Damageable_Com_C|GetFrozen _damageable)) (not (Variables|/Game/SpyroContent/Global_Assets/Global_Components/Damageable_Com.Damageable_Com_C|GetParalyzed_by_Fear _damageable)))
      (if (Variables|/Script/Engine.SceneComponent|GetbVisible (Variables|Default|Getspin_mesh))
        (Transformation|SetActorLocation (Math|Vector|Lerp(Vector) _returnvalue_2 (Math|Vector|MakeVector (select (Variables|Default|Getspinning%20home) (.x _spawn_point_2) (.x _spin_destination)) (select (Variables|Default|Getspinning%20home) (.y _spawn_point_2) (.y _spin_destination)) (.Z (Math|Vector|BreakVector _returnvalue_2))) (* (* (Utilities|Select :Index (Variables|Default|GetMy%20Current%20Difficulty) :NewEnumerator4 _medium_walk_speed :NewEnumerator0 (Variables|Default|GetEasy%20Walk%20Speed) :NewEnumerator1 _medium_walk_speed :NewEnumerator2 (Variables|Default|GetHard%20Walk%20Speed) :NewEnumerator3 (Variables|Default|GetNightmare%20Walk%20Speed)) 0.01) (Utilities|Time|GetWorldDeltaSeconds))) true false)
        (if (and (Math|Vector|Equal(Vector) _returnvalue_3 (Math|Vector|MakeVector (.x _spin_destination_2) (.y _spin_destination_2) (.Z (Math|Vector|BreakVector _returnvalue_3))) 2e+01) (not (Variables|Default|Getspinning%20home)))
          (Variables|Default|Setspinning%20home true)
          (elif (and (Math|Vector|Equal(Vector) _returnvalue (Math|Vector|MakeVector (.x _spawn_point) (.y _spawn_point) (.Z (Math|Vector|BreakVector _returnvalue))) 2e+01) (Variables|Default|Getspinning%20home))
            (Variables|Default|Setspinning%20home false))))
      (elif (Math|Boolean|ANDBoolean (Utilities|Enum|Equal(Enum) (Variables|/Game/SpyroContent/Global_Assets/Global_Components/Base_AI_Character.Base_AI_Character_C|GetAICharacter_State (Variables|Default|GetWalking_AI_Character)) "NewEnumerator2") (Variables|/Game/SpyroContent/Global_Assets/Global_Components/Damageable_Com.Damageable_Com_C|GetParalyzed_by_Fear (Variables|Default|GetDamageable)) (Utilities|Enum|Equal(Enum) (Variables|/Game/SpyroContent/Global_Assets/Global_Components/Damageable_Com.Damageable_Com_C|GetDamage_Being_Taken (Variables|Default|GetDamageable)) "NewEnumerator8"))
        (Default|ChangeAICharacterState _walking_ai_character_3 "NewEnumerator0")
        (Variables|/Game/SpyroContent/Global_Assets/Global_Components/Base_AI_Character.Base_AI_Character_C|SetAICharacter_State _walking_ai_character_3 "NewEnumerator0")
        (CallFunction|PenguinStateChanged)))))

(fn ConstructionScript
  (|CallParentFunction))

(fn SpinDamage
  (bind _returnvalue (Transformation|GetActorLocation))
  (bind _outhits (Collision|MultiSphereTraceForObjects _returnvalue _returnvalue 1e+02 (Utilities|Array|MakeArray "ObjectTypeQuery3" "ObjectTypeQuery9" "ObjectTypeQuery10" "ObjectTypeQuery8") false 0 "None"))
  (for _array_element _outhits
    (Utilities|IsValid (Actor|GetComponentbyClass (.hitactor _array_element) "/Game/SpyroContent/Global_Assets/Global_Components/Damageable_Com.Damageable_Com_C")
      (:Is%20Valid
        (if (Math|Boolean|ANDBoolean (Utilities|Enum|Equal(Enum) (Variables|/Game/SpyroContent/Global_Assets/Global_Components/Base_AI_Character.Base_AI_Character_C|GetAICharacter_State (Variables|Default|GetWalking_AI_Character)) "NewEnumerator2") (Variables|/Script/Engine.SceneComponent|GetbVisible (Variables|Default|Getspin_mesh)) (not (Variables|/Game/SpyroContent/Global_Assets/Global_Components/Damageable_Com.Damageable_Com_C|GetFrozen (Variables|Default|GetDamageable))))
          (Default|DealDamage (Actor|GetComponentbyClass (.hitactor _array_element) "/Game/SpyroContent/Global_Assets/Global_Components/Damageable_Com.Damageable_Com_C") "NewEnumerator4" (Transformation|GetActorForwardVector) false self false))))))