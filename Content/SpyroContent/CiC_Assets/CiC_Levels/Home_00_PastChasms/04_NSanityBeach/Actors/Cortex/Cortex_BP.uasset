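; Cortex NPC boss for N. Sanity Beach that starts flying and attacking once its dialogue ends.
; Self-looping delayed events pick random spline points and trigger AnimBP shooting, while Tick lerps toward the target, faces the player and projects a drop shadow.
; Successful damage stops attacks and talk, activates character movement and changes NPC state.
; Freezing also halts attacks, then sphere-traces for the surrounding ice block to make it invincible.
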(event Custom|start%20flying%20around
  (Utilities|FlowControl|DoOnce false
    (:Completed
      (Variables|Default|SetAttacking true)
      (CallFunction|RandomNewLocation)
      (CallFunction|RandomShoot))))

(event Custom|random%20new%20location
  (Utilities|FlowControl|Delay (Math|Random|RandomFloatinRange 0.5 2.0))
  (CallFunction|FindANewFlyTarget)
  (if (Variables|Default|GetAttacking)
    (CallFunction|RandomNewLocation)))

(event Custom|random%20shoot
  (if (Variables|Default|GetAttacking)
    (Utilities|FlowControl|Delay (Math|Random|RandomFloatinRange 0.5 2.0))
    (bind _ascortex_abp (Utilities|Casting|CastToCortex_ABP (Components|SkeletalMesh|GetAnimInstance (Variables|Character|GetMesh))))
    (if (not (Variables|/Game/SpyroContent/CiC_Assets/CiC_Levels/Home_00_PastChasms/04_NSanityBeach/Actors/Cortex/Cortex_ABP.Cortex_ABP_C|GetABP_Shooting _ascortex_abp))
      (Variables|/Game/SpyroContent/CiC_Assets/CiC_Levels/Home_00_PastChasms/04_NSanityBeach/Actors/Cortex/Cortex_ABP.Cortex_ABP_C|SetABP_Shooting _ascortex_abp true))))

(event Custom|cortex%20defeated
  (bind _returnvalue (Transformation|GetActorLocation))
  (bind _ascortex_abp (Utilities|Casting|CastToCortex_ABP (Components|SkeletalMesh|GetAnimInstance (Variables|Character|GetMesh))))
  (if (not (Variables|/Game/SpyroContent/CiC_Assets/CiC_Levels/Home_00_PastChasms/04_NSanityBeach/Actors/Cortex/Cortex_ABP.Cortex_ABP_C|Getcortex_hurt _ascortex_abp))
    (Utilities|FlowControl|Delay 0.5)
    (if (Variables|/Game/SpyroContent/Global_Assets/Global_Components/Damageable_Com.Damageable_Com_C|GetFrozen (Variables|Default|GetNPC_Damageable))
      (Variables|Default|SetAttacking false)
      (Variables|Default|SetAutotalks false)
      (bind _outhits (Collision|MultiSphereTraceForObjects _returnvalue _returnvalue 2e+02 (Utilities|Array|MakeArray "ObjectTypeQuery1") false 0 "None"))
      (for _array_element _outhits
        (if (.bblockinghit _array_element)
          (Utilities|FlowControl|DoOnce false
            (:Completed
              (bind _asice_block_bp (Utilities|Casting|CastToIce_Block_BP (.hitactor _array_element)))
              (Variables|/Game/SpyroContent/Global_Assets/Global_Components/Damageable_Com.Damageable_Com_C|SetInvincible (Variables|/Game/SpyroContent/Global_Assets/Global_Level_Items/Dragon_Breath/Blueprints/Ice_Block/Blueprints/Ice_Block_BP.Ice_Block_BP_C|GetDamageable _asice_block_bp) true)
              (Variables|/Game/SpyroContent/Global_Assets/Global_Components/Damageable_Com.Damageable_Com_C|SetObject's%20Hitbox%20Component (Variables|/Game/SpyroContent/Global_Assets/Global_Level_Items/Dragon_Breath/Blueprints/Ice_Block/Blueprints/Ice_Block_BP.Ice_Block_BP_C|GetDamageable _asice_block_bp) 0))))))))

(event EventBeginPlay
  (bind _npc_damageable (Variables|Default|GetNPC_Damageable))
  (|CallParentFunction)
  (Variables|Default|Setfly%20to%20here (Transformation|GetActorLocation))
  (EventDispatchers|BindEventtoDoneTalking (delegate Custom|start%20flying%20around))
  (EventDispatchers|BindEventtoCallFreeze _npc_damageable (delegate Custom|cortex%20defeated))
  (EventDispatchers|BindEventtoDamageWasSuccessfullyDealt _npc_damageable (delegate cortexishurt)))

(event EventTick
  (params (DeltaSeconds :type Float%20%28single-precision%29))
  (bind _npc_damageable (Variables|Default|GetNPC_Damageable))
  (|dropshadow
    (:then_1
      (|lookatplayer
        (:then_1
          (if (Math|Boolean|ANDBoolean (not (Variables|/Game/SpyroContent/Global_Assets/Global_Components/Damageable_Com.Damageable_Com_C|GetFrozen _npc_damageable)) (not (Variables|/Game/SpyroContent/Global_Assets/Global_Components/Damageable_Com.Damageable_Com_C|GetParalyzed_by_Fear _npc_damageable)) (not (Math|Vector|Equal(Vector) (Transformation|GetActorLocation) (Variables|Default|Getfly%20to%20here) 0.1)) (Variables|Default|GetAttacking))
            (Transformation|SetActorLocation (Math|Vector|Lerp(Vector) (Transformation|GetActorLocation) (Variables|Default|Getfly%20to%20here) (Utilities|Time|GetWorldDeltaSeconds)) true false)))))))

(fn ConstructionScript
  (|CallParentFunction))

(fn FindANewFlyTarget
  (bind _spline (Variables|Default|GetSpline))
  (Variables|Default|Setfly%20to%20here (Spline|GetLocationatDistanceAlongSpline _spline (Math|Random|RandomFloatinRange (Spline|GetDistanceAlongSplineatSplinePoint _spline 0) (Spline|GetDistanceAlongSplineatSplinePoint _spline 1)) "World")))

(event Custom|cortex%20hurt
  (if (not (Variables|/Game/SpyroContent/Global_Assets/Global_Components/Damageable_Com.Damageable_Com_C|GetFrozen (Variables|Default|GetNPC_Damageable)))
    (bind _ascortex_abp (Utilities|Casting|CastToCortex_ABP (Components|SkeletalMesh|GetAnimInstance (Variables|Character|GetMesh)))
      (:then
        (Variables|/Game/SpyroContent/CiC_Assets/CiC_Levels/Home_00_PastChasms/04_NSanityBeach/Actors/Cortex/Cortex_ABP.Cortex_ABP_C|Setcortex_hurt _ascortex_abp true))
      (:CastFailed
        _))
    (Variables|Default|SetAttacking false)
    (Variables|Default|SetAutotalks false)
    (Variables|Default|SetWon't%20Talk true)
    (Components|Activation|SetActive (Variables|Character|GetCharacterMovement) true false)
    (Utilities|FlowControl|Delay 0.2)
    (Variables|Default|SetNPC_State "NewEnumerator3")))