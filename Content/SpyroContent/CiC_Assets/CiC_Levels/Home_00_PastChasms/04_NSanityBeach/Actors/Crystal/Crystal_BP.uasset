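; Crystal pickup actor for the N. Sanity Beach level, collected when the playable character touches it.
; A Box overlap casts the other actor to BP_Base_Playable and accepts only contact from its capsule component.
; On pickup it spawns a rainbow burst just above itself, fires the CrystalCollected dispatcher for any listeners, plays the Crash Bandicoot crystal sound and destroys itself.
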(event OnComponentBeginOverlap(Box)
  (params (OverlappedComponent :type Primitive%20Component%20Object%20Reference) (OtherActor :type Actor%20Object%20Reference) (OtherComp :type Primitive%20Component%20Object%20Reference) (OtherBodyIndex :type Integer) (bFromSweep :type Boolean) (SweepResult :type Hit%20Result%20Structure%20%28by%20ref%29))
  (bind _returnvalue (Transformation|GetActorLocation))
  (bind _asbp_base_playable (Utilities|Casting|CastToBP_Base_Playable OtherActor))
  (if (== (Variables|/Script/Engine.Character|GetCapsuleComponent _asbp_base_playable) OtherComp)
    (Effects|SpawnEmitteratLocation "/Game/SpyroContent/Global_Assets/Global_Characters/NPCs/Bianca/Particles/Rainbow_Burst.Rainbow_Burst" (Math|Vector|MakeVector (.x _returnvalue) (.y _returnvalue) (+ (.z _returnvalue) 5e+01)))
    (Default|CallCrystalCollected)
    (Audio|PlaySoundatLocation "/Game/SpyroContent/CiC_Assets/CiC_Levels/Home_00_PastChasms/04_NSanityBeach/Audio/Crash_Bandicoot_Crystal.Crash_Bandicoot_Crystal" (Transformation|GetActorLocation) "0, 0, 0" 1.0 1.0 0.0 0 0 0)
    (Actor|DestroyActor)))

(event EventBeginPlay)

(event Collision|EventActorBeginOverlap
  (params (OtherActor :type Actor%20Object%20Reference)))

(event EventTick
  (params (DeltaSeconds :type Float%20%28single-precision%29)))

(fn ConstructionScript)