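; Monarch butterfly actor for N. Sanity Beach that flies along its own spline in a loop.
; BeginPlay pins the spline in world space, then Tick advances a wrapped distance by FlySpeed and sweeps the actor's location along it.
; Movement pauses while the Damageable component reports frozen or paralyzed by fear.
; Freezing shrinks the hitbox and melting restores it, with a repeating timer re-syncing its scale to the frozen state.
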(event Custom|frozen
  (if (Utilities|Enum|Equal(Enum) (Variables|/Game/SpyroContent/Global_Assets/Global_Components/Damageable_Com.Damageable_Com_C|GetDamage_Being_Taken (Variables|Default|GetDamageable)) "NewEnumerator7")
    (Transformation|SetRelativeScale3D (Variables|Default|Gethitbox) "0.100000,0.100000,0.100000")))

(event Custom|unfrozen
  (Transformation|SetRelativeScale3D (Variables|Default|Gethitbox) "1.000000,1.000000,1.000000"))

(event EventBeginPlay
  (bind _spline (Variables|Default|GetSpline))
  (|CallParentFunction)
  (Variables|/Game/SpyroContent/Global_Assets/Global_Components/Damageable_Com.Damageable_Com_C|SetObject's%20Hitbox%20Component (Variables|Default|GetDamageable) (Variables|Default|Gethitbox))
  (bind _output_get (Variables|Default|SetSpline%20Transform (Transformation|GetWorldTransform (Variables|Default|GetSpline))))
  (Transformation|SetAbsolute _spline true true true)
  (Transformation|SetWorldTransform _spline _output_get false false)
  (Transformation|SetActorLocation (Spline|GetLocationatSplinePoint _spline 6 "World") false false)
  (EventDispatchers|BindEventtoCallDealDamage (Variables|Default|GetDamageable) (delegate Custom|frozen))
  (EventDispatchers|BindEventtoMeltedfromIce (Variables|Default|GetDamageable) (delegate Custom|unfrozen))
  (Utilities|Time|SetTimerbyFunctionName 0 "hitbox check" 0.5 true))

(event EventTick
  (params (DeltaSeconds :type Float%20%28single-precision%29))
  (bind _damageable (Variables|Default|GetDamageable))
  (bind _spline (Variables|Default|GetSpline))
  (bind _returnvalue (Spline|GetSplineLength _spline))
  (|CallParentFunction DeltaSeconds)
  (if (Math|Boolean|ANDBoolean (not (Variables|/Game/SpyroContent/Global_Assets/Global_Components/Damageable_Com.Damageable_Com_C|GetFrozen _damageable)) (not (Variables|/Game/SpyroContent/Global_Assets/Global_Components/Damageable_Com.Damageable_Com_C|GetParalyzed_by_Fear _damageable)) (!= (Variables|Default|GetFly%20Speed) 0.0))
    (Variables|Default|SetDistance (select (> (+ (* (Utilities|Time|GetWorldDeltaSeconds) (Variables|Default|GetFly%20Speed)) (Variables|Default|GetDistance)) _returnvalue) 0.0 (select (< (+ (* (Utilities|Time|GetWorldDeltaSeconds) (Variables|Default|GetFly%20Speed)) (Variables|Default|GetDistance)) 0.0) _returnvalue (+ (* (Utilities|Time|GetWorldDeltaSeconds) (Variables|Default|GetFly%20Speed)) (Variables|Default|GetDistance)))))
    (Transformation|SetActorLocation (.location (Spline|GetTransformatDistanceAlongSpline (Variables|Default|GetSpline) (Variables|Default|GetDistance) "World" false)) true false)))

(fn ConstructionScript
  (|CallParentFunction))

(fn HitboxCheck
  (bind _damageable (Variables|Default|GetDamageable))
  (bind _frozen (Variables|/Game/SpyroContent/Global_Assets/Global_Components/Damageable_Com.Damageable_Com_C|GetFrozen _damageable))
  (bind _returnvalue (select _frozen 0.1 1.0))
  (Transformation|SetRelativeScale3D (Variables|Default|Gethitbox) (Math|Vector|MakeVector _returnvalue _returnvalue _returnvalue)))