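; Base Blueprint for a treasure chest that topples and breaks when the player's capsule overlaps its box in a specific player state and facing angle.
; The overlap switches the player's state, then a timeline tips the chest forward before a recursive Delay loop drops it a set distance and deals super damage through its Damageable component.
; Damage hides the gem, and an item dropper reset restores the gem and starting transform.
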(event DamageWasSuccessfullyDealt(Damageable)
  (Rendering|SetVisibility (Variables|Default|GetGemMesh) false false)
  (Variables|Default|SetToppleChestDestroyed true))

(event ItemDropperSuccessfullyReset(Item_Drop_Component)
  (Rendering|SetVisibility (Variables|Default|GetGemMesh) true false)
  (if (Variables|Default|GetToppleChestDestroyed)
    (Variables|Default|SetToppleChestDestroyed false)
    (Transformation|SetWorldLocationAndRotation (Variables|Default|GetRoot) (Variables|Default|GetInitialLocation) (Variables|Default|GetInitialRotation) false false)
    (Variables|Default|SetFallenDistance 0.0)))

(event DamageWasAttempted(Damageable))

(event OnComponentBeginOverlap(Box)
  (params (OverlappedComponent :type Primitive%20Component%20Object%20Reference) (OtherActor :type Actor%20Object%20Reference) (OtherComp :type Primitive%20Component%20Object%20Reference) (OtherBodyIndex :type Integer) (bFromSweep :type Boolean) (SweepResult :type Hit%20Result%20Structure%20%28by%20ref%29))
  (bind _returnvalue (Transformation|GetActorLocation))
  (bind _returnvalue_2 (Transformation|GetActorLocation OtherActor))
  (bind _returnvalue_3 (Transformation|GetActorForwardVector OtherActor))
  (bind _returnvalue_4 (- _returnvalue _returnvalue_2))
  (bind _returnvalue_5 (Math|Vector|Normalize _returnvalue_4))
  (bind _returnvalue_6 (Math|Vector|DotProduct _returnvalue_5 _returnvalue_3))
  (bind _returnvalue_7 (Class|KismetMathLibrary|DegAcos _returnvalue_6))
  (bind _asbp_base_playable (Utilities|Casting|CastToBP_Base_Playable OtherActor))
  (if (Math|Boolean|ANDBoolean (== (Variables|/Script/Engine.Character|GetCapsuleComponent _asbp_base_playable) OtherComp) (Utilities|Enum|Equal(Enum) (Variables|/Game/SpyroContent/Global_Assets/Global_Characters/Playable_Characters/BP_Base_Playable.BP_Base_Playable_C|GetPlayer_State _asbp_base_playable) "NewEnumerator4") (<= (- (Math|Float|MakeLiteralFloat 25.0) (Variables|Default|GetAngleTolerance)) _returnvalue_7) (>= (+ (Math|Float|MakeLiteralFloat 25.0) (Variables|Default|GetAngleTolerance)) _returnvalue_7))
    (Variables|/Game/SpyroContent/Global_Assets/Global_Characters/Playable_Characters/BP_Base_Playable.BP_Base_Playable_C|SetPlayer_State _asbp_base_playable "NewEnumerator5")
    (CallFunction|FallingSequence1)))

(event Custom|Falling%20Sequence%201
  (bind _returnvalue (Utilities|Time|GetWorldDeltaSeconds))
  (bind _root (Variables|Default|GetRoot))
  (bind _returnvalue_2 (Transformation|GetWorldTransform _root))
  (bind (_location _rotation) (Math|Transform|BreakTransform _returnvalue_2))
  (bind (_roll _pitch _yaw) (Math|Rotator|BreakRotator _rotation))
  (if (not (Variables|Default|GetToppleChestDestroyed))
    (Variables|Default|SetToppleChestDestroyed true)
    (bind (_direction _location_x _rotation__y) (Timeline|Timeline_3 PlayFromStart)
      (:Update
        (Transformation|SetWorldLocationAndRotation (Variables|Default|GetRoot) (+ (* (Transformation|GetActorForwardVector) (* (* (* _location_x _returnvalue) 1.2e+02) (Variables|Default|GetForwardTravelMultiplier))) _location) (Math|Rotator|MakeRotator _roll (+ (* (* _rotation__y _returnvalue) 1.2e+02) _pitch) _yaw) false false))
      (:Finished
        (CallFunction|FallingSequence2)))))

(event Custom|Falling%20Sequence%202
  (bind _returnvalue (Utilities|Time|GetWorldDeltaSeconds))
  (bind _root (Variables|Default|GetRoot))
  (bind _fallingspeed (Variables|Default|GetFallingSpeed))
  (bind _returnvalue_2 (Transformation|GetWorldLocation _root))
  (bind _returnvalue_3 (* _fallingspeed _returnvalue))
  (bind (_x _y _z) (Math|Vector|BreakVector _returnvalue_2))
  (bind _returnvalue_4 (* _returnvalue_3 1.2e+02))
  (if (<= (Variables|Default|GetFallingDistance) (Variables|Default|GetFallenDistance))
    (Default|DealDamage (Variables|Default|GetDamageable) "NewEnumerator4" "0, 0, 0" true 0 false)
    (else
      (Transformation|SetWorldLocation (Variables|Default|GetRoot) (Math|Vector|MakeVector _x _y (- _z _returnvalue_4)) false false)
      (Variables|Default|SetFallenDistance (+ (Variables|Default|GetFallenDistance) _returnvalue_4))
      (Utilities|FlowControl|Delay 0.008333)
      (CallFunction|FallingSequence2))))

(event EventBeginPlay
  (bind _root (Variables|Default|GetRoot))
  (bind _returnvalue (Transformation|GetWorldTransform _root))
  (bind (_location _rotation) (Math|Transform|BreakTransform _returnvalue))
  (|CallParentFunction)
  (Variables|Default|SetInitialLocation _location)
  (Variables|Default|SetInitialRotation _rotation))

(fn ConstructionScript
  (|CallParentFunction))