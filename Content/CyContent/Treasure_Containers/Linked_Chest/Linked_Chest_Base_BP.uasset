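; Base treasure chest that is linked to others sharing its Set and only breaks open once all are activated within a time limit.
; A damage attempt activates a chest, showing looping rotating rays and particles; the first one hit starts a one-second-step countdown.
; Full activation drops invincibility and deals super damage to every linked chest, crediting the player.
; Timeout deactivates the set, while an item dropper reset also restores invincibility.
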(event DamageWasAttempted(Damageable)
  (if (not (Variables|Default|GetIs%20Being%20Destroyed))
    (if (not (Variables|Default|GetActivated))
      (Rendering|SetVisibility (Variables|Default|GetRays) true false)
      (Components|Activation|Activate (Variables|Default|GetParticleSystem) false)
      (Variables|Default|SetActivated true)
      (CallFunction|ActivateTimer)
      (CallFunction|CheckifAllLinkedChestsAreActivated))))

(event ItemDropperSuccessfullyReset(Item_Drop_Component)
  (Variables|/Game/SpyroContent/Global_Assets/Global_Components/Damageable_Com.Damageable_Com_C|SetInvincible (Variables|Default|GetDamageable) true)
  (Variables|Default|SetIs%20Being%20Destroyed false)
  (Rendering|SetVisibility (Variables|Default|GetRays) false false)
  (Components|Activation|Deactivate (Variables|Default|GetParticleSystem))
  (Variables|Default|SetActivated false)
  (Variables|Default|SetInterrupt%20Timer true)
  (Variables|Default|SetTime%20Left -1)
  (CallFunction|Reset)
  (Variables|Default|SetI%20Was%20Activted%20First false)
  (Variables|Default|SetIs%20Being%20Destroyed false))

(event DamageWasSuccessfullyDealt(Damageable)
  (Rendering|SetVisibility (Variables|Default|GetRays) false false)
  (Components|Activation|Deactivate (Variables|Default|GetParticleSystem)))

(event Custom|Destroy%20Linked%20Chests
  (bind _outactors (Actor|GetAllActorsOfClass "Linked_Chest_Base_BP_C"))
  (for _array_element _outactors
    (if (== (Variables|Linked_Chest_Base_BP_C|GetSet _array_element) (Variables|Default|GetSet))
      (Variables|/Game/SpyroContent/Global_Assets/Global_Components/Damageable_Com.Damageable_Com_C|SetInvincible (Variables|/Game/SpyroContent/Global_Assets/Global_Level_Items/Treasure_Containers/Treasure_Container_Base_BP.Treasure_Container_Base_BP_C|GetDamageable _array_element) false)
      (Variables|Linked_Chest_Base_BP_C|SetIs%20Being%20Destroyed _array_element true)
      (bind _returnvalue (Actor|GetActorOfClass "/Game/SpyroContent/Global_Assets/Global_Characters/Playable_Characters/BP_Base_Playable.BP_Base_Playable_C"))
      (Default|DealDamage (Variables|/Game/SpyroContent/Global_Assets/Global_Level_Items/Treasure_Containers/Treasure_Container_Base_BP.Treasure_Container_Base_BP_C|GetDamageable _array_element) "NewEnumerator4" (Transformation|GetActorForwardVector _returnvalue) true _returnvalue true))))

(event Custom|Manage%20Timer
  (if (Variables|Default|GetInterrupt%20Timer)
    (Variables|Default|SetInterrupt%20Timer false)
    (elif (== (- (Variables|Default|GetTime%20Left) 1) 0)
      (bind _outactors (Actor|GetAllActorsOfClass "Linked_Chest_Base_BP_C"))
      (for _array_element _outactors
        (if (== (Variables|Linked_Chest_Base_BP_C|GetSet _array_element) (Variables|Default|GetSet))
          (CallFunction|DeactivateChest _array_element)))
      (else
        (Variables|Default|SetTime%20Left (- (Variables|Default|GetTime%20Left) 1))
        (Utilities|FlowControl|Delay 1.0)
        (CallFunction|ManageTimer)))))

(event Custom|Deactivate%20Chest
  (Rendering|SetVisibility (Variables|Default|GetRays) false false)
  (Components|Activation|Deactivate (Variables|Default|GetParticleSystem))
  (Variables|Default|SetActivated false)
  (Variables|Default|SetInterrupt%20Timer true)
  (Variables|Default|SetTime%20Left -1)
  (CallFunction|Reset)
  (Variables|Default|SetI%20Was%20Activted%20First false)
  (Variables|Default|SetIs%20Being%20Destroyed false))

(event Custom|Activate%20Timer
  (bind _outactors (Actor|GetAllActorsOfClass "Linked_Chest_Base_BP_C"))
  (for _array_element _outactors
    (if (== (Variables|Linked_Chest_Base_BP_C|GetSet _array_element) (Variables|Default|GetSet))
      (if (Variables|Linked_Chest_Base_BP_C|GetI%20Was%20Activted%20First _array_element)
        (Utilities|FlowControl|DoOnce false
          (:Completed
            (Variables|Default|SetTime%20Left (Variables|Linked_Chest_Base_BP_C|GetTime%20Left _array_element)))))))
  (if (== (Variables|Default|GetTime%20Left) -1)
    (Variables|Default|SetTime%20Left (Variables|Default|GetTimer))
    (Variables|Default|SetI%20Was%20Activted%20First true)
    (Variables|Default|SetInterrupt%20Timer false)
    (Utilities|FlowControl|Delay 1.0)
    (CallFunction|ManageTimer)))

(event Custom|Reset
  (Utilities|FlowControl|DoOnce false) ; enters at Reset
)

(event Custom|Check%20If%20All%20Linked%20Chests%20Are%20Activated
  (Variables|Default|SetNumber%20of%20Linked%20Chests 0)
  (Variables|Default|SetNumber%20of%20Activated%20Linked%20Chests 0)
  (bind _outactors (Actor|GetAllActorsOfClass "Linked_Chest_Base_BP_C"))
  (for _array_element _outactors
    (if (== (Variables|Linked_Chest_Base_BP_C|GetSet _array_element) (Variables|Default|GetSet))
      (Variables|Default|SetNumber%20of%20Linked%20Chests (+ (Variables|Default|GetNumber%20of%20Linked%20Chests) 1))
      (if (Variables|Linked_Chest_Base_BP_C|GetActivated _array_element)
        (Variables|Default|SetNumber%20of%20Activated%20Linked%20Chests (+ (Variables|Default|GetNumber%20of%20Activated%20Linked%20Chests) 1)))))
  (if (== (Variables|Default|GetNumber%20of%20Linked%20Chests) (Variables|Default|GetNumber%20of%20Activated%20Linked%20Chests))
    (CallFunction|DestroyLinkedChests)))

(event Custom|Rotate%20Rays
  (bind _newtrack_0 (Timeline|Timeline_3 PlayFromStart)
    (:Update
      (Transformation|SetRelativeRotation (Variables|Default|GetRays) (Math|Rotator|MakeRotator 0.0 0.0 _newtrack_0) false false))
    (:Finished
      (CallFunction|RotateRays))))

(event EventBeginPlay
  (|CallParentFunction)
  (CallFunction|RotateRays))

(fn ConstructionScript
  (|CallParentFunction))