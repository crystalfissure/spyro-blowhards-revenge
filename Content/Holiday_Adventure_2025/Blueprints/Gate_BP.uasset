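; Gate_BP is a gem-locked gate that shows its unlock cost on a child Gold_Text actor and opens when the player has enough gems.
; Tick reads the gem count from the HUD widget and fires OpenGate once through a DoOnce.
; Opening plays a sound and particle effect, then teleports the gate far below the level rather than destroying it.
; ResetGate restores the start location and re-arms the DoOnce; a debug flag opens it at BeginPlay.
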(event Custom|Open%20Gate
  (bind _sound___vfx_origin (Variables|Default|GetSound%20&%20VFX%20Origin))
  (bind _returnvalue (Transformation|GetWorldLocation _sound___vfx_origin))
  (Audio|PlaySoundatLocation (Variables|Default|GetGate%20unlock%20SFX) _returnvalue "0, 0, 0" 1.0 1.0 0.0 "/Game/SpyroContent/Global_Assets/Global_Audio/Attenuation/Spyro_Attenuation_Farther.Spyro_Attenuation_Farther" 0 0)
  (Effects|SpawnEmitteratLocation "/Game/Holiday_Adventure_2025/VFX/Gate_Cleared.Gate_Cleared" _returnvalue "0, 0, 0" "2.000000,2.000000,2.000000")
  (Transformation|SetActorLocation "0, 0,-50000.000000" false false))

(event Custom|Reset%20Gate
  (Transformation|SetActorLocation (Variables|Default|GetInitial%20Location) false false)
  (CallFunction|Reset))

(event Custom|Reset
  (Utilities|FlowControl|DoOnce false) ; enters at Reset
)

(event EventBeginPlay
  (Variables|Default|SetInitial%20Location (Transformation|GetActorLocation))
  (bind _asgold_text (Utilities|Casting|CastToGold_Text (Variables|/Script/Engine.ChildActorComponent|GetChildActor (Variables|Default|GetChildActor))))
  (Default|SetText _asgold_text (Utilities|String|ToString(Integer) (Variables|Default|GetGems%20to%20unlock)))
  (Variables|/Game/SpyroContent/Global_Assets/Global_Level_Items/Golden_Text/Gold_Text.Gold_Text_C|SetNever%20Hide _asgold_text true)
  (for _array_element (Actor|GetComponentsByClass _asgold_text "/Script/Engine.StaticMeshComponent")
    (Rendering|SetVisibility _array_element true false))
  (if (Variables|Default|GetDEBUG%20Despawn%20at%20Begin%20Play)
    (CallFunction|OpenGate)))

(event EventTick
  (params (DeltaSeconds :type Float%20%28single-precision%29))
  (bind _foundwidgets (Widget|GetAllWidgetsOfClass "/Game/SpyroContent/Global_Assets/Global_UserInterface/Widgets/HUD.HUD_C" true))
  (if (>= (Variables|/Game/SpyroContent/Global_Assets/Global_UserInterface/Widgets/HUD.HUD_C|GetActual_HUD_Gems (Utilities|Array|Get(acopy) _foundwidgets)) (Variables|Default|GetGems%20to%20unlock))
    (Utilities|FlowControl|DoOnce false
      (:Completed
        (CallFunction|OpenGate)))))

(fn ConstructionScript)