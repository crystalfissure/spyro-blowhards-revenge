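; Garland Blueprint that progressively spawns a line of Garland_Piece_BP actors along a spline, started by the Spawngarland event after a delay or by a debug option at BeginPlay.
; A looping timer runs the spawning sequence, advancing along the spline by a fixed spacing and clearing itself past the spline's end.
; Each piece gets a random gem mesh with its index-matched material, plus a matching particle burst at its location.
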(event Custom|Spawning%20sequence
  (bind _spline (Variables|Default|GetSpline))
  (bind _meshlist (Variables|Default|GetMeshList))
  (if (<= (Variables|Default|GetCurrentDistance) (Spline|GetSplineLength (Variables|Default|GetSpline)))
    (bind _returnvalue (Game|SpawnActorfromClass "/Game/Holiday_Adventure_2025/Blueprints/Garland_Piece_BP.Garland_Piece_BP_C" (Math|Transform|MakeTransform (Spline|GetLocationatDistanceAlongSpline _spline (Variables|Default|GetCurrentDistance) "World") (Spline|GetRotationatDistanceAlongSpline _spline (Variables|Default|GetCurrentDistance) "World") (Variables|Default|GetSpawn%20Transform%20Scale)) "Undefined" 0 0))
    (Variables|Default|SetInt (Math|Random|RandomIntegerinRange 0 (Utilities|Array|LastIndex _meshlist)))
    (Components|StaticMesh|SetStaticMesh (Variables|/Game/Holiday_Adventure_2025/Blueprints/Garland_Piece_BP.Garland_Piece_BP_C|GetGem%20Mesh _returnvalue) (Utilities|Array|Get(acopy) _meshlist (Variables|Default|GetInt)))
    (Rendering|Material|SetMaterial (Variables|/Game/Holiday_Adventure_2025/Blueprints/Garland_Piece_BP.Garland_Piece_BP_C|GetGem%20Mesh _returnvalue) 0 (Utilities|Array|Get(acopy) (Variables|Default|GetMaterialList) (Variables|Default|GetInt)))
    (Effects|SpawnEmitteratLocation (Utilities|Array|Get(acopy) (Variables|Default|GetParticleList) (Variables|Default|GetInt)) (Spline|GetLocationatDistanceAlongSpline _spline (Variables|Default|GetCurrentDistance) "World") (Spline|GetRotationatDistanceAlongSpline _spline (Variables|Default|GetCurrentDistance) "World"))
    (Variables|Default|SetCurrentDistance (+ (Variables|Default|GetCurrentDistance) (Variables|Default|GetSpacing)))
    (else
      (Utilities|Time|ClearandInvalidateTimerbyHandle (Variables|Default|GetSpawnTimerHandle)))))

(event Custom|Spawn%20garland
  (params (Delay :type Float%20%28single-precision%29))
  (Utilities|FlowControl|Delay Delay)
  (bind _returnvalue (Utilities|Time|SetTimerbyEvent (delegate Custom|Spawning%20sequence) (Variables|Default|GetSpawnInterval) true))
  (Variables|Default|SetSpawnTimerHandle _returnvalue))

(event EventBeginPlay
  (if (Variables|Default|GetDEBUG%20Spawn%20at%20begin%20play)
    (Utilities|FlowControl|Delay (Variables|Default|GetDEBUG%20Begin%20play%20spawn%20delay))
    (bind _returnvalue (Utilities|Time|SetTimerbyEvent (delegate Custom|Spawning%20sequence) (Variables|Default|GetSpawnInterval) true))
    (Variables|Default|SetSpawnTimerHandle _returnvalue)))

(fn ConstructionScript)