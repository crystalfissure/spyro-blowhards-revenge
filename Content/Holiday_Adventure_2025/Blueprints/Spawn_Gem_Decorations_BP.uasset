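; Holiday Adventure actor that reveals pre-placed gem decorations one at a time in random order.
; After a start delay, it gathers all Gem_Decoration_Base_BP actors and shuffles the array.
; A self-calling event makes each gem visible at a set interval, then fires the DoneSpawning dispatcher when no valid entry remains.
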(event Custom|Start%20spawning%20decorations
  (params (Delay :type Float%20%28single-precision%29))
  (Utilities|FlowControl|Delay Delay)
  (bind _outactors (Actor|GetAllActorsOfClass "/Game/Holiday_Adventure_2025/Blueprints/Gem_Decoration_Base_BP.Gem_Decoration_Base_BP_C"))
  (Variables|Default|SetOut%20Actors _outactors)
  (CallFunction|ShuffleArray))

(event Custom|Spawn%20Decorations
  (bind _index (Variables|Default|GetIndex))
  (bind _out_actors (Variables|Default|GetOut%20Actors))
  (bind _output (Utilities|Array|Get(acopy) _out_actors _index))
  (Utilities|IsValid _output
    (:Is%20Valid
      (Default|MakeGemVisible _output)
      (Math|Integer|IncrementInt _index
        (:%20%20
          (Utilities|FlowControl|Delay (Variables|Default|GetInterval))
          (CallFunction|SpawnDecorations))))
    (:Is%20Not%20Valid
      (Default|CallDoneSpawning))))

(event Custom|Shuffle%20array
  (Utilities|Array|Shuffle (Variables|Default|GetOut%20Actors))
  (CallFunction|SpawnDecorations))

(event EventBeginPlay)

(event Collision|EventActorBeginOverlap
  (params (OtherActor :type Actor%20Object%20Reference)))

(event EventTick
  (params (DeltaSeconds :type Float%20%28single-precision%29)))

(fn ConstructionScript)