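; Base gem decoration actor for the holiday adventure, hidden until it is revealed.
; BeginPlay hides GemMesh and, if RandomizeRotation is set, gives it a random yaw, with pitch flipped unless it is a cyan gem.
; The Makegemvisible event shows the mesh and spawns a particle burst at the VFXSpawnLocation component.
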(event Custom|Make%20gem%20visible
  (Rendering|SetVisibility (Variables|Default|GetGem%20Mesh) true false)
  (Effects|SpawnEmitteratLocation (Variables|Default|GetEmitter%20Template) (Transformation|GetWorldLocation (Variables|Default|GetVFX%20Spawn%20Location)) "0, 0, 0" "2.000000,2.000000,2.000000"))

(event EventBeginPlay
  (Rendering|SetVisibility (Variables|Default|GetGem%20Mesh) false false)
  (if (Variables|Default|GetRandomize%20rotation)
    (Transformation|SetRelativeRotation (Variables|Default|GetGem%20Mesh) (Math|Rotator|MakeRotator 0.0 (select (Variables|Default|GetIs%20cyan%20gem) (Math|Float|MakeLiteralFloat 0.0) (Math|Float|MakeLiteralFloat 1.8e+02)) (Math|Random|RandomFloatinRange 0.0 3.6e+02)) false false)))

(event Collision|EventActorBeginOverlap
  (params (OtherActor :type Actor%20Object%20Reference)))

(event EventTick
  (params (DeltaSeconds :type Float%20%28single-precision%29)))

(fn ConstructionScript)