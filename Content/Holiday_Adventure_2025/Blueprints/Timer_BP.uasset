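; Timer_BP runs a gem-collection challenge whose difficulty is chosen through NPC dialogue, setting skill level and, on Normal and above, a countdown.
; Gem pickups, container hits and enemy damage add time to a looping 0.1-second timer that updates the widget.
; Reaching the gem total teleports the player to Moneybags; untimed modes poll for this.
; Timeout freezes players, then resets gates, gems and positions and returns to the NPC.
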(event Custom|Start%20Countdown
  (params (StartTime :type Float%20%28single-precision%29))
  (Variables|Default|SetTime%20Remaining StartTime)
  (Default|ShowTimer (Variables|Default|GetTimer%20Widget))
  (bind _returnvalue (Utilities|Time|SetTimerbyEvent (delegate Custom|Tick%20Timer) 0.1 true))
  (Variables|Default|SetTimer%20Handle _returnvalue)
  (Variables|/Game/SpyroContent/Global_Assets/Global_Characters/NPCs/NPC_Base_BP.NPC_Base_BP_C|SetWon't%20Talk (Variables|Default|GetNPC%20Ref) true)
  (bind _outactors (Actor|GetAllActorsOfClass "/Game/SpyroContent/Global_Assets/Global_Characters/Playable_Characters/BP_Base_Playable.BP_Base_Playable_C"))
  (for (_array_element _array_index) _outactors
    (if (> _array_index 0)
      (bind _asspyro_player_controller (Utilities|Casting|CastToSpyro_PlayerController (Pawn|GetController _array_element)))
      (Input|EnableInput _array_element _asspyro_player_controller)
      (Variables|/Game/SpyroContent/Global_Assets/Global_Characters/Playable_Characters/BP_Base_Playable.BP_Base_Playable_C|SetDid%20we%20disable%20input? _array_element false))))

(event Custom|Tick%20Timer
  (bind _output_get (Variables|Default|SetTime%20Remaining (- (Variables|Default|GetTime%20Remaining) 0.1)))
  (if (<= _output_get 0.0)
    (Utilities|Time|ClearandInvalidateTimerbyHandle (Variables|Default|GetTimer%20Handle))
    (Development|PrintString "Timer's up!")
    (Default|UpdateTime (Variables|Default|GetTimer%20Widget) 0.0)
    (Default|ShowWidget (Variables|Default|GetTime's%20up%20Widget))
    (bind _outactors (Actor|GetAllActorsOfClass "/Game/SpyroContent/Global_Assets/Global_Characters/Playable_Characters/BP_Base_Playable.BP_Base_Playable_C"))
    (for _array_element _outactors
      (bind _asspyro_player_controller (Utilities|Casting|CastToSpyro_PlayerController (Pawn|GetController _array_element)))
      (Input|DisableInput _array_element _asspyro_player_controller)
      (Variables|/Game/SpyroContent/Global_Assets/Global_Characters/Playable_Characters/BP_Base_Playable.BP_Base_Playable_C|SetDid%20we%20disable%20input? _array_element true)
      (Components|Movement|StopMovementImmediately (Variables|/Script/Engine.Character|GetCharacterMovement _array_element))
      (Character|StopJumping _array_element))
    (Utilities|FlowControl|Delay 2.0)
    (CallFunction|ResetLevel)
    (else
      (Default|UpdateTime (Variables|Default|GetTimer%20Widget) (Variables|Default|GetTime%20Remaining))
      (bind _foundwidgets (Widget|GetAllWidgetsOfClass "/Game/SpyroContent/Global_Assets/Global_UserInterface/Widgets/HUD.HUD_C" true))
      (if (>= (Variables|/Game/SpyroContent/Global_Assets/Global_UserInterface/Widgets/HUD.HUD_C|GetActual_HUD_Gems (Utilities|Array|Get(acopy) _foundwidgets)) (Variables|Default|GetTotal%20gems))
        (Utilities|Time|ClearandInvalidateTimerbyHandle (Variables|Default|GetTimer%20Handle))
        (Default|HideTimer (Variables|Default|GetTimer%20Widget))
        (CallFunction|TeleporttoMoneybags)))))

(event Custom|Add%20time%20when%20defeating%20enemies
  (CallFunction|AddTime (Variables|Default|Get+%20Time%20for%20each%20gem%20collected)))

(event Custom|Freeroam%20Difficulty%20Chosen
  (Variables|Default|SetTimer%20enabled false)
  (Variables|/Game/SpyroContent/Global_Assets/Global_Characters/NPCs/NPC_Base_BP.NPC_Base_BP_C|SetWon't%20Talk (Variables|Default|GetNPC%20Ref) true)
  (CallFunction|NoTimerMoneybagsCheck)
  ;[0 0 0] There's no way to set skill level so we need to do subtractions and additions here
  (CallFunction|UpdateSkillLevel -1e+02 self)
  (bind _outactors (Actor|GetAllActorsOfClass "/Game/Holiday_Adventure_2025/Blueprints/Gate_BP.Gate_BP_C"))
  (for _array_element _outactors
    (Default|OpenGate _array_element)))

(event Custom|Show%20record
  (bind _returnvalue (UserInterface|CreateWidget "/Game/Holiday_Adventure_2025/UI/Finished_In_Widget.Finished_In_Widget_C"))
  (UserInterface|Viewport|AddtoViewport _returnvalue 0)
  (Default|UpdateText _returnvalue (Variables|Default|GetTime%20Remaining)))

(event Custom|Nightmare%20Difficulty%20Chosen
  (Variables|Default|SetStart%20time (Variables|Default|GetStart%20time%20Nightmare))
  (Variables|Default|Set+%20Time%20for%20each%20gem%20collected (Variables|Default|Get+%20Time%20for%20each%20gem%20collected%20Nightmare))
  ;[0 0 0] There's no way to set skill level so we need to do subtractions and additions here
  (CallFunction|UpdateSkillLevel 1e+02 self)
  (Variables|Default|SetTimer%20enabled true))

(event Custom|Reset%20Level
  (bind _npc_ref (Variables|Default|GetNPC%20Ref))
  (Default|HideWidget (Variables|Default|GetTime's%20up%20Widget))
  (Default|HideTimer (Variables|Default|GetTimer%20Widget))
  (Variables|/Game/SpyroContent/Global_Assets/Global_Characters/NPCs/NPC_Base_BP.NPC_Base_BP_C|SetWon't%20Talk _npc_ref false)
  (Variables|/Game/SpyroContent/Global_Assets/Global_Characters/NPCs/NPC_Base_BP.NPC_Base_BP_C|SetDialogue_Info _npc_ref (Variables|Default|GetDialogue%20Info))
  (bind _outactors (Actor|GetAllActorsOfClass "/Game/SpyroContent/Global_Assets/Global_Characters/Playable_Characters/BP_Base_Playable.BP_Base_Playable_C"))
  (for (_array_element _array_index) _outactors
    (Variables|/Game/SpyroContent/Global_Assets/Global_Characters/Playable_Characters/BP_Base_Playable.BP_Base_Playable_C|SetPowerUp_Time_Remaining _array_element 0.0)
    (if (== _array_index 0)
      (Default|Melt (Variables|/Game/SpyroContent/Global_Assets/Global_Characters/Playable_Characters/BP_Base_Playable.BP_Base_Playable_C|GetDamageable _array_element))
      (Default|TeleporttoTalktoMe (Variables|Default|GetNPC%20Ref) _array_element 0.5)
      (else
        (Transformation|SetActorLocation _array_element (Utilities|Select :Index _array_index :Option%200 "0, 0, 0" :Option%201 (Transformation|GetWorldLocation (Variables|Default|GetPlayer%202%20Spawn%20Location)) :Option%202 (Transformation|GetWorldLocation (Variables|Default|GetPlayer%203%20Spawn%20Location)) :Option%203 (Transformation|GetWorldLocation (Variables|Default|GetPlayer%204%20Spawn%20Location))) false false))))
  (Utilities|FlowControl|Delay 0.5)
  (Utilities|FlowControl|Sequence
    (:then_0
      (bind _outactors_2 (Actor|GetAllActorsOfClass "/Game/Holiday_Adventure_2025/Blueprints/Gate_BP.Gate_BP_C"))
      (for _array_element_2 _outactors_2
        (Default|ResetGate _array_element_2)))
    (:then_1
      (bind _outactors_3 (Actor|GetAllActorsOfClass "/Game/ExampleAdventure/Utils/BP_Yeetwind_Spawner.BP_Yeetwind_Spawner_C"))
      (for _array_element_3 _outactors_3
        (Default|HideHurlwind _array_element_3)))
    (:then_2
      (bind _asspyro_persistant_data (Utilities|Casting|CastToSpyro_PersistantData (Game|GetGameInstance)))
      (Default|CallResetGems _asspyro_persistant_data))))

(event Custom|Restore%20input%20for%20other%20players
  (bind _outactors (Actor|GetAllActorsOfClass "/Game/SpyroContent/Global_Assets/Global_Characters/Playable_Characters/BP_Base_Playable.BP_Base_Playable_C"))
  (for (_array_element _array_index) _outactors
    (if (> _array_index 0)
      (bind _asspyro_player_controller (Utilities|Casting|CastToSpyro_PlayerController (Pawn|GetController _array_element)))
      (Input|EnableInput _array_element _asspyro_player_controller)
      (Variables|/Game/SpyroContent/Global_Assets/Global_Characters/Playable_Characters/BP_Base_Playable.BP_Base_Playable_C|SetDid%20we%20disable%20input? _array_element false))))

(event Custom|Teleport%20to%20Moneybags
  (bind _moneybags_ref (Variables|Default|GetMoneybags%20Ref))
  (Variables|/Game/SpyroContent/Global_Assets/Global_Characters/NPCs/NPC_Base_BP.NPC_Base_BP_C|SetWon't%20Talk _moneybags_ref false)
  (bind _returnvalue (Actor|GetActorOfClass "/Game/SpyroContent/Global_Assets/Global_Characters/Playable_Characters/BP_Base_Playable.BP_Base_Playable_C"))
  (Default|TeleporttoTalktoMe _moneybags_ref _returnvalue 0.5))

(event Custom|Add%20Time
  (params (TimeToAdd :type Float%20%28single-precision%29))
  (Variables|Default|SetTime%20Remaining (+ TimeToAdd (Variables|Default|GetTime%20Remaining))))

(event Custom|Hard%20Difficulty%20Chosen
  (bind _self self)
  (Variables|Default|SetStart%20time (Variables|Default|GetStart%20time%20Hard))
  (Variables|Default|Set+%20Time%20for%20each%20gem%20collected (Variables|Default|Get+%20Time%20for%20each%20gem%20collected%20Hard))
  ;[0 0 0] There's no way to set skill level so we need to do subtractions and additions here
  (CallFunction|UpdateSkillLevel -1e+02 _self)
  (CallFunction|UpdateSkillLevel 85.0 _self)
  (Variables|Default|SetTimer%20enabled true))

(event Custom|Add%20time%20when%20destroying%20treasure%20containers
  (CallFunction|AddTime (Variables|Default|Get+%20Time%20for%20each%20gem%20collected)))

(event Custom|Start%20the%20Timer
  (if (Variables|Default|GetTimer%20enabled)
    (CallFunction|StartCountdown (Variables|Default|GetStart%20time))
    (else
      (CallFunction|RestoreInputforOtherPlayers))))

(event Custom|Add%20time%20when%20collecting%20gems
  (CallFunction|AddTime (Variables|Default|Get+%20Time%20for%20each%20gem%20collected)))

(event Custom|Easy%20Difficulty%20Chosen
  (bind _self self)
  (Variables|Default|SetTimer%20enabled false)
  (Variables|/Game/SpyroContent/Global_Assets/Global_Characters/NPCs/NPC_Base_BP.NPC_Base_BP_C|SetWon't%20Talk (Variables|Default|GetNPC%20Ref) true)
  (CallFunction|NoTimerMoneybagsCheck)
  ;[0 0 0] There's no way to set skill level so we need to do subtractions and additions here
  (CallFunction|UpdateSkillLevel -1e+02 _self)
  (CallFunction|UpdateSkillLevel 25.0 _self))

(event Custom|No%20Timer%20Moneybags%20Check
  (bind _foundwidgets (Widget|GetAllWidgetsOfClass "/Game/SpyroContent/Global_Assets/Global_UserInterface/Widgets/HUD.HUD_C" true))
  (if (>= (Variables|/Game/SpyroContent/Global_Assets/Global_UserInterface/Widgets/HUD.HUD_C|GetActual_HUD_Gems (Utilities|Array|Get(acopy) _foundwidgets)) (Variables|Default|GetTotal%20gems))
    (CallFunction|TeleporttoMoneybags)
    (else
      (Utilities|FlowControl|Delay 0.5)
      (CallFunction|NoTimerMoneybagsCheck))))

(event Custom|Normal%20Difficulty%20Chosen
  (bind _self self)
  (Variables|Default|SetStart%20time (Variables|Default|GetStart%20time%20Normal))
  (Variables|Default|Set+%20Time%20for%20each%20gem%20collected (Variables|Default|Get+%20Time%20for%20each%20gem%20collected%20Normal))
  ;[0 0 0] There's no way to set skill level so we need to do subtractions and additions here
  (CallFunction|UpdateSkillLevel -1e+02 _self)
  (CallFunction|UpdateSkillLevel 3e+01 _self)
  (Variables|Default|SetTimer%20enabled true))

(event EventBeginPlay
  (bind _npc_ref (Variables|Default|GetNPC%20Ref))
  (Utilities|FlowControl|Sequence
    (:then_0
      (bind _returnvalue (UserInterface|CreateWidget "/Game/Holiday_Adventure_2025/UI/Time_Left_Widget.Time_Left_Widget_C"))
      (bind _output_get (Variables|Default|SetTimer%20Widget _returnvalue))
      (UserInterface|Viewport|AddtoViewport _output_get 0))
    (:then_1
      (bind _returnvalue_2 (UserInterface|CreateWidget "/Game/Holiday_Adventure_2025/UI/Times_Up_Widget.Times_Up_Widget_C"))
      (bind _output_get_2 (Variables|Default|SetTime's%20up%20Widget _returnvalue_2))
      (UserInterface|Viewport|AddtoViewport _output_get_2 0))
    (:then_2
      (EventDispatchers|BindEventtoOption0Chosen _npc_ref (delegate Custom|Freeroam%20Difficulty%20Chosen))
      (EventDispatchers|BindEventtoOption1Chosen _npc_ref (delegate Custom|Easy%20Difficulty%20Chosen))
      (EventDispatchers|BindEventtoOption2Chosen _npc_ref (delegate Custom|Normal%20Difficulty%20Chosen))
      (EventDispatchers|BindEventtoOption3Chosen _npc_ref (delegate Custom|Hard%20Difficulty%20Chosen))
      (EventDispatchers|BindEventtoOption4Chosen _npc_ref (delegate Custom|Nightmare%20Difficulty%20Chosen))
      (EventDispatchers|BindEventtoDoneTalking (Variables|Default|GetNPC%20Ref) (delegate Custom|Start%20the%20Timer))
      (Variables|Default|SetDialogue%20Info (Variables|/Game/SpyroContent/Global_Assets/Global_Characters/NPCs/NPC_Base_BP.NPC_Base_BP_C|GetDialogue_Info (Variables|Default|GetNPC%20Ref)))
      (Utilities|FlowControl|Sequence
        (:then_0
          (bind _outactors (Actor|GetAllActorsOfClass "/Game/SpyroContent/Global_Assets/Global_Level_Items/Gems/Actors/Gem_Base_BP.Gem_Base_BP_C"))
          (for _array_element _outactors
            (EventDispatchers|BindEventtoGemWasCollected _array_element (delegate Custom|Add%20time%20when%20collecting%20gems))))
        (:then_1
          (bind _outactors_2 (Actor|GetAllActorsOfClass "/Game/SpyroContent/Global_Assets/Global_Level_Items/Treasure_Containers/Treasure_Container_Base_BP.Treasure_Container_Base_BP_C"))
          (for _array_element_2 _outactors_2
            (EventDispatchers|BindEventtoContainerSuccessfullyDamaged _array_element_2 (delegate Custom|Add%20time%20when%20destroying%20treasure%20containers))))
        (:then_2
          (bind _outactors_3 (Actor|GetAllActorsOfClass "/Game/SpyroContent/Global_Assets/Global_Characters/AI_Characters/Actors/Enemies/Base_Enemy_BP.Base_Enemy_BP_C"))
          (for _array_element_3 _outactors_3
            (EventDispatchers|BindEventtoDamageWasSuccessfullyDealt (Variables|/Game/SpyroContent/Global_Assets/Global_Characters/AI_Characters/Actors/Base_AICharacter_BP.Base_AICharacter_BP_C|GetDamageable _array_element_3) (delegate Custom|Add%20time%20when%20defeating%20enemies))))))))

(fn ConstructionScript)