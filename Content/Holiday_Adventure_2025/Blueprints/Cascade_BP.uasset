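; Cascade spawner that emits a stream of gem actors along a spline, with repeating sound effects.
; Start and stop events control two looping timers, one spawning gems at the spline start and one playing a 2D sound.
; Each gem receives the spline and movement speed, plus a random mesh and particle template paired by shared index.
; A debug flag starts the cascade at BeginPlay and stops it after a delay.
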(event Custom|Spawn%20gems
  (bind _meshlist (Variables|Default|GetMeshList))
  (bind _returnvalue (Game|SpawnActorfromClass "/Game/Holiday_Adventure_2025/Blueprints/Cascade_Gem_BP.Cascade_Gem_BP_C" (Math|Transform|MakeTransform (Spline|GetLocationatDistanceAlongSpline (Variables|Default|GetSpline) 0.0 "World") "0, 0, 0" "1,1,1") "Undefined" 0 (Variables|Default|GetSpline) (Variables|Default|GetMovementSpeed) 0))
  (Variables|Default|SetInt (Math|Random|RandomIntegerinRange 0 (Utilities|Array|LastIndex _meshlist)))
  (Components|StaticMesh|SetStaticMesh (Variables|/Game/Holiday_Adventure_2025/Blueprints/Cascade_Gem_BP.Cascade_Gem_BP_C|GetGem%20Mesh _returnvalue) (Utilities|Array|Get(acopy) _meshlist (Variables|Default|GetInt)))
  (Effects|Components|ParticleSystem|SetTemplate (Variables|/Game/Holiday_Adventure_2025/Blueprints/Cascade_Gem_BP.Cascade_Gem_BP_C|GetParticleSystem _returnvalue) (Utilities|Array|Get(acopy) (Variables|Default|GetParticleList) (Variables|Default|GetInt))))

(event Custom|Start%20spawning%20gems
  (bind _returnvalue (Utilities|Time|SetTimerbyEvent (delegate Custom|Spawn%20gems) (Variables|Default|GetSpawnInterval) true))
  (Variables|Default|SetTimerHandle _returnvalue)
  (bind _returnvalue_2 (Utilities|Time|SetTimerbyEvent (delegate Custom|Play%20SFX) (Variables|Default|GetSFX%20Interval) true))
  (Variables|Default|SetSFX%20Timer%20Handle _returnvalue_2))

(event Custom|Stop%20spawning%20gems
  (Utilities|Time|ClearandInvalidateTimerbyHandle (Variables|Default|GetTimerHandle))
  (Utilities|Time|ClearandInvalidateTimerbyHandle (Variables|Default|GetSFX%20Timer%20Handle)))

(event Custom|DEBUG%20Stop%20spawning%20after%20delay
  (Utilities|FlowControl|Delay (Variables|Default|GetDEBUG%20Stop%20spawning%20after%20X%20seconds))
  (Utilities|Time|ClearandInvalidateTimerbyHandle (Variables|Default|GetTimerHandle))
  (Utilities|Time|ClearandInvalidateTimerbyHandle (Variables|Default|GetSFX%20Timer%20Handle)))

(event Custom|Play%20SFX
  (Audio|PlaySound2D (Variables|Default|GetSFX) (Variables|Default|GetSFX%20Volume%20Multiplier) 1.0 0.0 0 0))

(event EventBeginPlay
  (if (Variables|Default|GetDEBUG%20Activate%20at%20Begin%20Play)
    (CallFunction|DEBUGStopSpawningAfterDelay)
    (bind _returnvalue (Utilities|Time|SetTimerbyEvent (delegate Custom|Spawn%20gems) (Variables|Default|GetSpawnInterval) true))
    (Variables|Default|SetTimerHandle _returnvalue)
    (bind _returnvalue_2 (Utilities|Time|SetTimerbyEvent (delegate Custom|Play%20SFX) (Variables|Default|GetSFX%20Interval) true))
    (Variables|Default|SetSFX%20Timer%20Handle _returnvalue_2)))

(fn ConstructionScript)