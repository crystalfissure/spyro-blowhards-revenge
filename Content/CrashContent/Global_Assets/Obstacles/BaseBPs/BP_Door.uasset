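; BP_Door is a two-panel sliding door obstacle that opens when the player enters its Box trigger and closes when they leave.
; Overlaps from a BP_Base_Playable capsule call Movedoor, which plays a tomb-door sound and runs a timeline forward to close or in reverse to open.
; The timeline slides the panels oppositely along local X, with multipliers for travel distance and speed.
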(event OnComponentBeginOverlap(Box)
  (params (OverlappedComponent :type Primitive%20Component%20Object%20Reference) (OtherActor :type Actor%20Object%20Reference) (OtherComp :type Primitive%20Component%20Object%20Reference) (OtherBodyIndex :type Integer) (bFromSweep :type Boolean) (SweepResult :type Hit%20Result%20Structure%20%28by%20ref%29))
  (bind _asbp_base_playable (Utilities|Casting|CastToBP_Base_Playable OtherActor))
  (if (== (Variables|/Script/Engine.Character|GetCapsuleComponent _asbp_base_playable) OtherComp)
    (CallFunction|MoveDoor false)))

(event OnComponentEndOverlap(Box)
  (params (OverlappedComponent :type Primitive%20Component%20Object%20Reference) (OtherActor :type Actor%20Object%20Reference) (OtherComp :type Primitive%20Component%20Object%20Reference) (OtherBodyIndex :type Integer))
  (bind _asbp_base_playable (Utilities|Casting|CastToBP_Base_Playable OtherActor))
  (if (== (Variables|/Script/Engine.Character|GetCapsuleComponent _asbp_base_playable) OtherComp)
    (CallFunction|MoveDoor true)))

(event Custom|Move%20door
  (params (Close%20door :type Boolean))
  (bind _door_travel_distance_multiplier (Variables|Default|GetDoor%20travel%20distance%20multiplier))
  (Audio|PlaySoundatLocation "/Game/CrashContent/SFX/SFX_TombDoor.SFX_TombDoor" (Transformation|GetActorLocation) "0, 0, 0" 1.0 1.0 0.0 "/Game/SpyroContent/Global_Assets/Global_Audio/Attenuation/Spyro_Attenuation_Farther.Spyro_Attenuation_Farther" 0 0)
  (if Close%20door
    (bind _newtrack_0 (Timeline|Timeline_0 Play)
      (:Update
        (Transformation|SetRelativeLocation (Variables|Default|GetRight%20door) (Math|Vector|MakeVector (* _newtrack_0 _door_travel_distance_multiplier) 0.0 0.0) false false)
        (Transformation|SetRelativeLocation (Variables|Default|GetLeft%20door) (* (Math|Vector|MakeVector (* _newtrack_0 _door_travel_distance_multiplier) 0.0 0.0) -1.0) false false)))
    (else
      (Timeline|Timeline_0 Reverse))))

(event EventBeginPlay
  (Components|Timeline|SetPlayRate (Variables|Default|GetTimeline_0) (Variables|Default|GetDoor%20speed%20multiplier)))

(fn ConstructionScript)