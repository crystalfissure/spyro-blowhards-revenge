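; BP_Falling_Platform_Looping is an obstacle platform that repeatedly falls on a timed loop.
; After an initial BeginPlay delay, a timeline drives the static mesh's relative Z location, scaled by FallingDistanceMultiplier.
; When the timeline finishes, it waits a configurable delay and replays from the start, moving without sweep and independently of player contact.
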(event Custom|ManageFallingPlatform
  (bind _newtrack_0 (Timeline|Timeline_0 PlayFromStart)
    (:Update
      (Transformation|SetRelativeLocation (Variables|Default|GetStaticMesh) (Math|Vector|MakeVector 0.0 0.0 (* (Variables|Default|GetFalling%20Distance%20Multiplier) _newtrack_0)) false false))
    (:Finished
      (Utilities|FlowControl|Delay (Variables|Default|GetDelay))
      (CallFunction|ManageFallingPlatform))))

(event EventBeginPlay
  (Utilities|FlowControl|Delay (Variables|Default|GetBeginPlayDelay))
  (CallFunction|ManageFallingPlatform))

(event Collision|EventActorBeginOverlap
  (params (OtherActor :type Actor%20Object%20Reference)))

(event EventTick
  (params (DeltaSeconds :type Float%20%28single-precision%29)))

(fn ConstructionScript)