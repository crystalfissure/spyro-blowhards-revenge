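; Travel platform that carries the player one way along a spline after they first step on it.
; The trigger overlap sets the player's ground state and, after a delay, starts a looping 120 Hz timer that advances the mesh by speed, with optional yaw following the spline.
; Fall-prevention colliders are enabled only during travel and switch off on arrival.
; The spline-camera branches are empty, and the stored initial location is unused here.
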(event OnComponentBeginOverlap(TriggerBox)
  (params (OverlappedComponent :type Primitive%20Component%20Object%20Reference) (OtherActor :type Actor%20Object%20Reference) (OtherComp :type Primitive%20Component%20Object%20Reference) (OtherBodyIndex :type Integer) (bFromSweep :type Boolean) (SweepResult :type Hit%20Result%20Structure%20%28by%20ref%29))
  (bind _asbp_base_playable (Utilities|Casting|CastToBP_Base_Playable OtherActor))
  (if (== (Variables|/Script/Engine.Character|GetCapsuleComponent _asbp_base_playable) OtherComp)
    (Variables|/Game/SpyroContent/Global_Assets/Global_Characters/Playable_Characters/BP_Base_Playable.BP_Base_Playable_C|SetGround_State _asbp_base_playable "NewEnumerator0")
    (if (not (Variables|Default|GetisActivated))
      (Variables|Default|SetisActivated true)
      (if (Variables|Default|GetSet%20Spline%20Camera)
        _
        (else
          _))
      (Utilities|FlowControl|Delay (Variables|Default|GetTravel%20Start%20Delay))
      (CallFunction|StartPlatformMovement _asbp_base_playable))))

(event Custom|Start%20Platform%20Movement
  (params (BP%20Base%20Playable%20Ref :type BP%20Base%20Playable%20Object%20Reference))
  (Variables|Default|SetisMoving true)
  (Utilities|Time|SetTimerbyFunctionName 0 "MovePlatform" 0.008333 true)
  (if (Variables|Default|GetSet%20Spline%20Camera)
    _
    (else
      _))
  (Collision|SetCollisionEnabled (Variables|Default|GetFallPrevention) "QueryAndPhysics"))

(event Custom|On%20Platform%20Arrived
  (Variables|Default|SetisMoving false)
  (Utilities|Time|ClearTimerbyFunctionName 0 "MovePlatform")
  (Collision|SetCollisionEnabled (Variables|Default|GetFallPrevention) "NoCollision"))

(event EventBeginPlay
  (Variables|Default|SetSplineLenght (Spline|GetSplineLength (Variables|Default|GetSplinePath)))
  (Collision|SetCollisionEnabled (Variables|Default|GetFallPrevention) "NoCollision")
  (Variables|Default|SetInitialLocation (Transformation|GetWorldLocation (Variables|Default|GetPlatformMesh))))

(fn ConstructionScript)

(fn MovePlatform
  (if (Variables|Default|GetisMoving)
    (Variables|Default|SetCurrentSplineDistance (+ (Variables|Default|GetCurrentSplineDistance) (* (Variables|Default|GetMovementSpeed) (Utilities|Time|GetWorldDeltaSeconds))))
    (if (>= (+ (Variables|Default|GetCurrentSplineDistance) (* (Variables|Default|GetMovementSpeed) (Utilities|Time|GetWorldDeltaSeconds))) (Variables|Default|GetSplineLenght))
      (CallFunction|OnPlatformArrived)
      (else
        (Transformation|SetWorldLocation (Variables|Default|GetPlatformMesh) (Spline|GetLocationatDistanceAlongSpline (Variables|Default|GetSplinePath) (Variables|Default|GetCurrentSplineDistance) "World") false false)
        (if (Variables|Default|GetRotate%20platform)
          (Transformation|SetRelativeRotation (Variables|Default|GetPlatformMesh) (Math|Rotator|MakeRotator 0.0 0.0 (+ (.Yaw (Math|Rotator|BreakRotator (Spline|GetRotationatDistanceAlongSpline (Variables|Default|GetSplinePath) (Variables|Default|GetCurrentSplineDistance) "World"))) (Variables|Default|GetPlatform%20rotation%20offset))) false false))))))